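; GM_TradeCity is the game mode for the TradeCity level, setting up shared state and registering joining Sky player controllers.
; A one-time custom begin-play step fetches the SGI object from the game instance and finds the PlayerIsland actor.
; That step runs from BeginPlay or the first new-player event, whichever comes first.
; Each new PC_Sky receives the island reference and joins the SGI player list.
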(event Custom|CustomBeginPlay
  (Variables|Default|SethadBeginPlayer true)
  (bind _sgi (Class|BPISGI|GetSGI(Message) (Game|GetGameInstance)))
  (Variables|Default|SetSGI _sgi)
  (bind _returnvalue (Actor|GetActorOfClass "/Game/Blueprints/PlayerIsland.PlayerIsland_C"))
  (Variables|Default|SetPlayerIsland _returnvalue))

(event EventBeginPlay
  (if (not (Variables|Default|GethadBeginPlayer))
    (CallFunction|CustomBeginPlay)))

(event EventHandleStartingNewPlayer
  (params (NewPlayer :type Player%20Controller%20Object%20Reference))
  (if (Variables|Default|GethadBeginPlayer)
    _
    (else
      (CallFunction|CustomBeginPlay)))
  (bind _aspc_sky (Utilities|Casting|CastToPC_Sky NewPlayer))
  (Variables|/Game/Blueprints/PC_Sky.PC_Sky_C|SetPlayerIsland _aspc_sky (Variables|Default|GetPlayerIsland))
  (Utilities|Array|Add (Variables|/Game/Blueprints/SGI.SGI_C|GetPlayers (Variables|Default|GetSGI)) _aspc_sky))

(fn ConstructionScript)