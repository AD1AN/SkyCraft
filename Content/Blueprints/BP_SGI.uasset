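; Game instance that handles multiplayer session hosting and joining and loads custom settings on init.
; Hosting creates an advanced session tagged with the world name, optionally unadvertised, then opens SkyMain as a listen server or restores the main menu on failure.
; Search results and accepted invites both join sessions directly.
; Server events run servertravel by console command and call ClientClearCWS on every tracked player.
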(event Custom|HostGame
  (params (bAllowJoinViaPresenceFriendsOnly :type Boolean))
  (bind _current_w_loadingscreen (Variables|Default|GetCurrent_W_LoadingScreen))
  (Utilities|Array|Clear (Variables|Default|GetPlayers))
  (|AdvancedSession (Utilities|Array|MakeArray (Class|AdvancedSessionsLibrary|MakeLiteralSessionPropertyString "WorldName" (Variables|Default|GetLoadWorldName))) (Game|GetPlayerController 0) 100 100 false true false true true true false false true (not bAllowJoinViaPresenceFriendsOnly) false true
    (:OnSuccess
      (Game|OpenLevel(byObjectReference) "/Game/Levels/SkyMain.SkyMain" true "?listen")
      (Variables|Default|SetExitedMainMenu true))
    (:OnFailure
      (Utilities|IsValid _current_w_loadingscreen
        (:Is%20Valid
          (Widget|RemovefromParent _current_w_loadingscreen))
        (:Is%20Not%20Valid
          _))
      (Utilities|Platform|CollectGarbage)
      (Input|SetInputModeGameandUI (Game|GetPlayerController 0) (Variables|Default|GetCurrent_W_MainMenu) "DoNotLock" false)
      (Widget|SetVisibility (Variables|Default|GetCurrent_W_MainMenu) "Visible"))))

(event Custom|OnlineJoinGame
  (params (SearchResult :type Blueprint%20Session%20Result%20Structure%20%28by%20ref%29))
  (|JoinSession (Game|GetPlayerController 0) SearchResult))

(event EventOnSessionInviteAccepted
  (params (LocalPlayerNum :type Integer) (PersonInvited :type BP%20Unique%20Net%20Id%20Structure) (SessionToJoin :type Blueprint%20Session%20Result%20Structure%20%28by%20ref%29))
  (|JoinSession (Game|GetPlayerController 0) SessionToJoin))

(event EventInit
  (bind _ssg_customsettings (CallFunction|LoadCustomSettings))
  (Variables|Default|SetCustomSettings _ssg_customsettings))

(event Custom|AllClientsClearCWS
  (for _array_element (Variables|Default|GetPlayers)
    (Default|ClientClearCWS _array_element)))

(event Custom|ServerTravel
  (params (Level%20Name :type String))
  (Development|ExecuteConsoleCommand (Utilities|String|Append "servertravel " Level%20Name) 0))