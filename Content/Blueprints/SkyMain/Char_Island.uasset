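; Char_Island is the player's island-form pawn, with camera turning, a HUD, inventory and island menus, and a hold-Jump action to emerge as a Char_Normal.
; A completed hold traces for ground ahead, then the server spawns the character, passes on essence, items and, in Sky Main, chunk generation.
; A multicast timeline moves spirit effects along a spline, after which the owning client requests the possession switch and this pawn is destroyed.
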(event Custom|Server_SpawnNormal
  (params (SpawnTransform :type Transform))
  (CallFunction|SpawnCharNormal (.location SpawnTransform) (.rotation SpawnTransform)))

(event Custom|Client_Possess
  (bind _pc_sky (Variables|Default|GetPC_Sky))
  (bind _pc_sky_2 (Variables|Default|GetPC_Sky))
  (bind _w_bstransition (Variables|/Game/Blueprints/SkyMain/PC_Sky.PC_Sky_C|GetW_BSTransition _pc_sky_2))
  (bind _returnvalue (UserInterface|CreateWidget "/Game/Widgets/W_CharIsland.W_CharIsland_C" _pc_sky _pc_sky self))
  (bind _output_get (Variables|Default|SetW_CharIsland _returnvalue))
  (UserInterface|Viewport|AddtoViewport _output_get 0)
  (Utilities|IsValid _w_bstransition
    (:Is%20Valid
      (Default|HideBlack _w_bstransition (delegate Custom|HideCompleted)))))

(event Custom|Client_SetRandomRotation
  (Pawn|SetControlRotation (Variables|Default|GetPC_Sky) (Math|Rotator|MakeRotator 0.0 0.0 (Math|Random|RandomFloatinRange 5.0 355.0))) ; If rotation default = wind sound is freaking
)

(event Custom|HideCompleted)

(event Custom|Multicast_SpiritSpawnAnimation
  (params (Char_IslandRotation :type Rotator))
  (bind _pc_sky (Variables|Default|GetPC_Sky))
  (Transformation|SetActorRotation Char_IslandRotation)
  (bind _move (Timeline|SpawnTimeline Play)
    (:Update
      (Transformation|SetRelativeLocation (Variables|Default|GetSpiritSpawn) (Spline|GetLocationatDistanceAlongSpline (Variables|Default|GetSpline) (Math|Float|Lerp 0.0 (Spline|GetSplineLength (Variables|Default|GetSpline)) _move) "Local") false false))
    (:Finished
      (Utilities|IsValid _pc_sky
        (:Is%20Valid
          (if (Variables|/Game/Blueprints/SkyMain/PC_Sky.PC_Sky_C|GetIAmOwner _pc_sky) ; If this character local player
            (CallFunction|ServerSwitch)))))))

(event Custom|Server_Switch
  (bind _pc_sky (Variables|Default|GetPC_Sky))
  (bind _pc_sky_2 (Variables|Default|GetPC_Sky))
  (bind _char_normal (Variables|/Game/Blueprints/SkyMain/PC_Sky.PC_Sky_C|GetChar_Normal _pc_sky_2))
  (Rendering|SetActorHiddenInGame _char_normal false)
  (CallFunction|MulticastDeactivate)
  (CallFunction|MulticastSNNormalSpawn _char_normal)
  (Pawn|Possess _pc_sky (Variables|/Game/Blueprints/SkyMain/PC_Sky.PC_Sky_C|GetChar_Normal _pc_sky))
  (Actor|DestroyActor))

(event Custom|Multicast_InitSetup
  (params (Essence :type S%20Essence%20Structure) (InventorySlots :type Array%20of%20S%20Inventory%20Slot%20Structures))
  (Variables|Default|SetEssence Essence)
  (Variables|/Game/Inventory/Inventory.Inventory_C|SetInventorySlots (Variables|Default|GetInventory) InventorySlots))

(event Custom|Multicast_Deactivate
  (bind _sn_spiritspawn (Variables|Default|GetSN_SpiritSpawn))
  (if (not (Networking|IsDedicatedServer))
    (Utilities|IsValid _sn_spiritspawn
      (:Is%20Valid
        (Default|DeactivateStazNiagara _sn_spiritspawn)))))

(event Custom|Multicast_SN_SpiritSpawn
  (if (not (Networking|IsDedicatedServer))
    (bind _returnvalue (Game|SpawnActorfromClass "/Game/Particles/StazNiagara.StazNiagara_C" (Math|Transform|MakeTransform "0, 0, 0" "0, 0, 0" "1.000000,1.000000,1.000000") "AlwaysSpawn" 0 "/Game/Particles/Char_Island_SpiritSpawn.Char_Island_SpiritSpawn" 0))
    (bind _output_get (Variables|Default|SetSN_SpiritSpawn _returnvalue))
    (Transformation|AttachComponentToComponent _output_get (Variables|Default|GetSpiritSpawn) "None" "KeepRelative" "KeepRelative" "KeepRelative" true)))

(event Custom|Multicast_SN_Normal_Spawn
  (params (ParentActor :type Actor%20Object%20Reference))
  (if (not (Networking|IsDedicatedServer))
    (bind _returnvalue (Game|SpawnActorfromClass "/Game/Particles/StazNiagara.StazNiagara_C" (Math|Transform|MakeTransform "0, 0, 0" "0, 0, 0" "1.000000,1.000000,1.000000") "AlwaysSpawn" 0 "/Game/Particles/Char_Normal_Spawn.Char_Normal_Spawn" 0))
    (Transformation|AttachActorToActor _returnvalue ParentActor "None" "KeepRelative" "KeepRelative" "KeepRelative" true)))

(event Custom|OnDestroyed_Event_0
  (params (DestroyedActor :type Actor%20Object%20Reference))
  (if (not (Variables|Default|GetEmerging))
    (Default|ServerPlayersInsideChange (Variables|Default|GetPC_Sky) -1)))

(event EventBeginPlay
  (bind _pc_sky (Variables|Default|GetPC_Sky))
  (bind _sgi (Class|BPISGI|GetSGI(Message) (Game|GetGameInstance)))
  (Variables|Default|SetSGI _sgi)
  (Utilities|FlowControl|Sequence
    (:then_0
      (Utilities|IsValid _pc_sky
        (:Is%20Valid
          (if (Variables|/Game/Blueprints/SkyMain/PC_Sky.PC_Sky_C|GetIAmOwner _pc_sky)
            (CallFunction|ClientSetRandomRotation)))))
    (:then_1
      (if (Networking|IsServer)
        (Game|AssignOnDestroyed (delegate Custom|OnDestroyed_Event_0))))))

(event EventPossessed
  (params (NewController :type Controller%20Object%20Reference))
  (Variables|/Game/Blueprints/SkyMain/PC_Sky.PC_Sky_C|SetPlayerForm (Variables|Default|GetPC_Sky) "NewEnumerator0")
  (CallFunction|ClientPossess)
  (Game|Player|SetViewTargetwithBlend (Variables|Default|GetPC_Sky) self 0.0 "VTBlend_Linear" 0.0 false))

(event Input|ActionEvents|InputActionJump
  (params (Key :type Key%20Structure))
  (bind _returnvalue (Transformation|GetActorRotation))
  (bind _returnvalue_2 (Transformation|GetActorLocation))
  (bind _emergeprogress (Variables|Default|GetEmergeProgress))
  (bind _returnvalue_3 (Math|Vector|GetForwardVector (Math|Rotator|MakeRotator 0.0 0.0 (.yaw _returnvalue))))
  (bind _returnvalue_4 (+ _returnvalue_2 "0, 0,100.000000"))
  (bind _returnvalue_5 (* _returnvalue_3 2e+02))
  (bind _returnvalue_6 (+ _returnvalue_4 _returnvalue_5))
  (:Pressed
    (Utilities|Hold/Tap 0.15 :!label _label
      (:HoldStart
        (if (Class|LowEntryExtendedStandardLibrary|ShippingBuild)
          (Components|Timeline|SetPlayRate _emergeprogress 1.0)
          (bind _progressvalue (Timeline|EmergeProgress PlayFromStart)
            (:Update
              (Default|SetProgress (Variables|/Game/Widgets/W_CharIsland.W_CharIsland_C|GetReviveProgress (Variables|Default|GetW_CharIsland)) _progressvalue))
            (:Finished
              (bind (_outhit _returnvalue_7) (Collision|LineTraceByChannel _returnvalue_6 (+ _returnvalue_6 "0, 0,-400.000000") "TraceTypeQuery1" false 0 "None"))
              (if _returnvalue_7
                (CallFunction|ServerSpawnNormal (Math|Transform|MakeTransform (+ (.Location (Collision|BreakHitResult _outhit)) "0, 0,100.000000") (Transformation|GetActorRotation)))
                (Widget|RemovefromParent (Variables|Default|GetW_CharIsland))
                (Input|DisableInput self (Variables|Default|GetPC_Sky))
                (else
                  (Default|SetProgress (Variables|/Game/Widgets/W_CharIsland.W_CharIsland_C|GetReviveProgress (Variables|Default|GetW_CharIsland)) 0.0)))))
          (else
            (Components|Timeline|SetPlayRate _emergeprogress 15.0)
            (Timeline|EmergeProgress PlayFromStart))))
      (:HoldStop
        (Default|SetProgress (Variables|/Game/Widgets/W_CharIsland.W_CharIsland_C|GetReviveProgress (Variables|Default|GetW_CharIsland)) 0.0)
        (Timeline|EmergeProgress Stop))))
  (:Released
    (goto _label Released)))

(event Input|ActionEvents|InputActionInteract
  (params (Key :type Key%20Structure))
  (bind _pc_sky (Variables|Default|GetPC_Sky))
  (:Pressed
    (bind _returnvalue (UserInterface|CreateWidget "/Game/Widgets/CWS/CWS_PlayerIsland.CWS_PlayerIsland_C" _pc_sky (Variables|/Game/Blueprints/SkyMain/PC_Sky.PC_Sky_C|GetPlayerIsland _pc_sky) _pc_sky self)) ; One more in Pawn_IslandControl(Interact)
    (UserInterface|Viewport|AddtoViewport _returnvalue 0)
    (Default|AddCWS (Variables|Default|GetPC_Sky) _returnvalue)
    (Default|SetMousetoCenter (Variables|Default|GetPC_Sky))))

(event Input|ActionEvents|InputActionInventory
  (params (Key :type Key%20Structure))
  (bind _pc_sky (Variables|Default|GetPC_Sky))
  (:Pressed
    (bind _returnvalue (UserInterface|CreateWidget "/Game/Widgets/CWS/CWS_InventoryCharIsland.CWS_InventoryCharIsland_C" _pc_sky _pc_sky self))
    (UserInterface|Viewport|AddtoViewport _returnvalue 0)
    (Default|AddCWS (Variables|Default|GetPC_Sky) _returnvalue)))

(event Input|AxisEvents|InputAxisLookUp
  (params (AxisValue :type Float%20%28single-precision%29))
  (bind _cameraboom (Variables|Default|GetCameraBoom))
  (bind _returnvalue (Transformation|GetWorldRotation _cameraboom))
  (Transformation|SetWorldRotation (Variables|Default|GetCameraBoom) (Math|Rotator|MakeRotator (.roll _returnvalue) (Math|Float|ClampAngle (+ (* AxisValue -1.0) (.pitch _returnvalue)) -5e+01 0.0) (.yaw _returnvalue)) false false))

(event Input|AxisEvents|InputAxisTurn
  (params (AxisValue :type Float%20%28single-precision%29))
  (bind _returnvalue (Transformation|GetActorRotation))
  (Transformation|SetActorRotation (Math|Rotator|MakeRotator (.roll _returnvalue) (.pitch _returnvalue) (+ AxisValue (.yaw _returnvalue)))))

(fn ConstructionScript)

(fn SpawnCharNormal
  (params (SpawnTransform_Location :type Vector) (Char_IslandRotation :type Rotator))
  (bind _pc_sky (Variables|Default|GetPC_Sky))
  (bind _returnvalue (Game|SpawnActorfromClass "/Game/Blueprints/SkyMain/Char_Normal.Char_Normal_C" (Math|Transform|MakeTransform SpawnTransform_Location (Math|Rotator|MakeRotator 0.0 0.0 (.Yaw (Math|Rotator|BreakRotator Char_IslandRotation))) "1.000000,1.000000,1.000000") "AdjustIfPossibleButAlwaysSpawn" _pc_sky _pc_sky (Variables|Default|GetPS_Sky) 0))
  (bind _output_get (LocalVariables|Set_Char_Normal _returnvalue))
  (Default|ClientSetLookRotation _output_get Char_IslandRotation)
  (Default|MulticastInitSetup (LocalVariables|Get_Char_Normal) (Variables|Default|GetEssence) (Variables|/Game/Inventory/Inventory.Inventory_C|GetInventorySlots (Variables|Default|GetInventory)) (Variables|/Game/Inventory/Inventory.Inventory_C|GetInventorySlots (Variables|Default|GetInventory_Equipment)))
  (Variables|Default|SetEmerging true)
  (Default|ServerPlayersInsideChange (Variables|Default|GetPC_Sky) -1)
  (switch Utilities|FlowControl|Switch|SwitchonCurrentLevel (Variables|/Game/Blueprints/SGI.SGI_C|GetCurrentLevel (Variables|Default|GetSGI))
    (:NewEnumerator1
      (Default|SpawnChunks (Variables|/Game/Blueprints/SkyMain/Char_Normal.Char_Normal_C|GetGenerator_Islands (LocalVariables|Get_Char_Normal)))
      (Default|MinusSpawnedChunks (Variables|Default|GetGenerator_Islands))
      (Default|SpawnChunks (Variables|/Game/Blueprints/SkyMain/Char_Normal.Char_Normal_C|GetGenerator_Essence (LocalVariables|Get_Char_Normal)))
      (Default|MinusSpawnedChunks (Variables|Default|GetGenerator_Essence)))
    (:NewEnumerator2
      _))
  (bind _output_get_2 (Variables|/Game/Blueprints/SkyMain/PC_Sky.PC_Sky_C|SetChar_Normal (Variables|Default|GetPC_Sky) (LocalVariables|Get_Char_Normal)))
  (Game|Player|SetViewTargetwithBlend (Variables|Default|GetPC_Sky) _output_get_2 1.0 "VTBlend_EaseInOut" 2.0 false)
  (CallFunction|MulticastSpiritSpawnAnimation Char_IslandRotation)
  (CallFunction|MulticastSNSpiritSpawn))

(fn OnRepEssence
  (Default|CallEssenceChanged))

(fn GetACInventory
  (return (Variables|Default|GetInventory)))

(fn GetCharNormal
  (return 0))

(fn GetGeneratorIslands
  (return (Variables|Default|GetGenerator_Islands)))

(fn GetPCSky
  (return 0))

(fn GetLookRotation
  (return (Variables|Default|GetLookRotation)))

(fn SetLookRotation
  (params (LookRotation :type Rotator :default "0, 0, 0"))
  (bind _output_get (Variables|Default|SetLookRotation LookRotation))
  (return _output_get))