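; Player pawn for the dead state, holding the player's Essence and inventory while they orbit the camera and watch a lifespan countdown.
; The server ticks and multicasts the lifespan; expiry, or pressing E, fades to black and respawns the player as an island character.
; Other players can open its inventory or revive the owner as a Char_Normal with those contents.
; Once unpossessed, the body is destroyed when emptied or expired.
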(event AfterUnpossessed(AfterPossessed)
  (bind _w_chardead (Variables|Default|GetW_CharDead))
  (Utilities|IsValid _w_chardead
    (:Is%20Valid
      (Widget|RemovefromParent _w_chardead))
    (:Is%20Not%20Valid
      _))
  (Utilities|IsValid (Variables|Default|GetW_CharDeadInsideInventory)
    (:Is%20Valid
      (Widget|RemovefromParent (Variables|Default|GetW_CharDeadInsideInventory))
      (Variables|Default|SetW_CharDeadInsideInventory 0) ; empty
    )
    (:Is%20Not%20Valid
      _))
  (Utilities|Platform|CollectGarbage)
  (Actor|Tick|SetActorTickEnabled false))

(event Custom|Server_Respawn
  (params (Destroy :type Boolean))
  (bind _essence (Variables|Default|GetEssence))
  (Default|MulticastClearEditablewith (Variables|Default|GetAC_Interact))
  (bind _spawned_char_island (Default|SpawnCharIsland (Variables|Default|GetPC_Sky) true))
  (Default|SpawnChunks (Variables|/Game/Blueprints/SkyMain/Char_Island.Char_Island_C|GetGenerator_Islands _spawned_char_island)) ; Force Spawn Chunks to avoid re-spawn
  (Default|MinusSpawnedChunks (Variables|Default|GetGenerator_Islands))
  (Default|SpawnChunks (Variables|/Game/Blueprints/SkyMain/Char_Island.Char_Island_C|GetGenerator_Essence _spawned_char_island)) ; Force Spawn Chunks to avoid re-spawn
  (Default|MinusSpawnedChunks (Variables|Default|GetGenerator_Essence))
  (if Destroy
    (CallFunction|ServerSideDestroyCharDead)
    (else
      (Variables|/Game/Blueprints/SkyMain/PC_Sky.PC_Sky_C|SetChar_Dead (Variables|Default|GetPC_Sky) 0) ; empty
      (Variables|Default|SetPC_Sky 0) ; empty
      (if (and (== (Utilities|Array|Length (Variables|/Game/Inventory/AC_Inventory.AC_Inventory_C|GetInventory (Variables|Default|GetAC_Inventory))) 0) (== (+ (.red _essence) (.green _essence) (.blue _essence)) 0))
        (CallFunction|ServerSideDestroyCharDead)))))

(event Custom|Client_Possessed
  (bind _returnvalue (UserInterface|CreateWidget "/Game/Widgets/W_CharDead.W_CharDead_C" (Variables|Default|GetPC_Sky) self))
  (bind _output_get (Variables|Default|SetW_CharDead _returnvalue))
  (UserInterface|Viewport|AddtoViewport _output_get 0)
  (Actor|Tick|SetActorTickEnabled true))

(event Custom|ServerSide_DestroyCharDead
  (CallFunction|MulticastLOCALWOutside)
  (Actor|DestroyActor))

(event Custom|REMOVE_Inventory_Event_0
  (params (RemovedIndex :type Integer))
  (bind _essence (Variables|Default|GetEssence))
  (Utilities|IsValid (Variables|Default|GetPC_Sky)
    (:Is%20Not%20Valid
      (if (and (<= (+ (.red _essence) (.green _essence) (.blue _essence)) 0) (== (Utilities|Array|Length (Variables|/Game/Inventory/AC_Inventory.AC_Inventory_C|GetInventory (Variables|Default|GetAC_Inventory))) 0))
        (CallFunction|ServerSideDestroyCharDead)))))

(event Custom|Multicast_LOCAL_W_Outside
  (bind _local_cws_chardeadoutsideinventory (Variables|Default|GetLOCAL_CWS_CharDeadOutsideInventory))
  (Utilities|IsValid _local_cws_chardeadoutsideinventory
    (:Is%20Valid
      (Default|ClientSideDestroyWidget _local_cws_chardeadoutsideinventory))))

(event Custom|Multicast_SetCurrentLifeSpan%28Unreliable%29
  (params (CurrentLifeSpan :type Float%20%28double-precision%29))
  (Variables|Default|SetCurrentLifeSpan CurrentLifeSpan))

(event Custom|Client_SetLookRotation
  (params (LookRotation :type Rotator))
  (bind _output_get (Variables|Default|SetLookRotation LookRotation))
  (Transformation|SetWorldRotation (Variables|Default|GetSpringArm) _output_get false false))

(event Custom|Multicast_SetLookRotation%28Reliable%29
  (params (LookRotation :type Rotator))
  (bind _output_get (Variables|Default|SetLookRotation LookRotation))
  (Transformation|SetWorldRotation (Variables|Default|GetSpringArm) _output_get false false))

(event Custom|2ShowBlackCompleted
  (CallFunction|ServerRespawn true))

(event Custom|ShowBlackCompleted
  (CallFunction|ServerRespawn false))

(event Custom|EssenceChanged_Event_0
  (bind _essence (Variables|Default|GetEssence))
  (Utilities|IsValid (Variables|Default|GetPC_Sky)
    (:Is%20Not%20Valid
      (if (and (<= (+ (.red _essence) (.green _essence) (.blue _essence)) 0) (== (Utilities|Array|Length (Variables|/Game/Inventory/AC_Inventory.AC_Inventory_C|GetInventory (Variables|Default|GetAC_Inventory))) 0))
        (CallFunction|ServerSideDestroyCharDead)))))

(event Custom|Client_EndLifeSpan
  (Default|CreateWBSTransition (Variables|Default|GetPC_Sky) (delegate Custom|2ShowBlackCompleted)))

(event Custom|Server_EndLifeSpan
  (Utilities|IsValid (Variables|Default|GetPC_Sky)
    (:Is%20Valid
      (CallFunction|ClientEndLifeSpan))
    (:Is%20Not%20Valid
      (CallFunction|ServerSideDestroyCharDead))))

(event Custom|Mutlicast_InitSetup
  (params (Essence :type S%20Essence%20Structure) (Inventory :type Array%20of%20S%20Inventory%20Slot%20Structures))
  (Variables|Default|SetEssence Essence)
  (Variables|/Game/Inventory/AC_Inventory.AC_Inventory_C|SetInventory (Variables|Default|GetAC_Inventory) Inventory))

(event EventPossessed
  (params (NewController :type Controller%20Object%20Reference))
  (Variables|/Game/Blueprints/SkyMain/PC_Sky.PC_Sky_C|SetPlayerForm (Variables|Default|GetPC_Sky) "NewEnumerator1")
  (CallFunction|ClientPossessed)
  (Game|Player|SetViewTargetwithBlend (Variables|Default|GetPC_Sky) self 0.0 "VTBlend_Linear" 0.0 false)
  (Actor|Tick|SetActorTickEnabled true))

(event EventBeginPlay
  (if (Networking|IsServer)
    (EventDispatchers|AssignEssenceChanged (delegate Custom|EssenceChanged_Event_0))
    (EventDispatchers|AssignREMOVEInventory (Variables|Default|GetAC_Inventory) (delegate Custom|REMOVE_Inventory_Event_0))))

(event EventTick
  (params (DeltaSeconds :type Float%20%28single-precision%29))
  (bind _w_chardead (Variables|Default|GetW_CharDead))
  (bind _pc_sky (Variables|Default|GetPC_Sky))
  (Utilities|FlowControl|Sequence
    (:then_0
      (if (Networking|IsServer)
        (if (<= (Variables|Default|GetCurrentLifeSpan) 0.0)
          (Utilities|FlowControl|DoOnce false
            (:Completed
              (CallFunction|ServerEndLifeSpan)))
          (else
            (bind _output_get (Variables|Default|SetCurrentLifeSpan (- (Variables|Default|GetCurrentLifeSpan) (Utilities|Time|GetWorldDeltaSeconds))))
            (CallFunction|MulticastSetCurrentLifeSpan(Unreliable) _output_get)))))
    (:then_1
      (Utilities|IsValid _pc_sky
        (:Is%20Valid
          (if (Variables|/Game/Blueprints/SkyMain/PC_Sky.PC_Sky_C|GetIAmOwner _pc_sky) ; If this character local player
            (Transformation|SetWorldRotation (Variables|Default|GetSpringArm) (Variables|Default|GetLookRotation) false false)
            (Default|SetProgress (Variables|/Game/Widgets/W_CharDead.W_CharDead_C|GetDissolveProgress _w_chardead) (/ (Variables|Default|GetCurrentLifeSpan) (Variables|Default|GetMaxLifeSpan)))
            (Rendering|Components|TextRender|SetText (Variables|/Game/Widgets/W_CharDead.W_CharDead_C|GetRemainLifeSpan _w_chardead) (Utilities|Text|FormatText "{0}:{1}" (Utilities|Text|ToText(Integer) (Math|Timespan|GetMinutes (Math|Timespan|MakeTimespan 0 0 0 (Math|Float|Truncate (Variables|Default|GetCurrentLifeSpan)) 0)) false true 2 2) (Utilities|Text|ToText(Integer) (Math|Timespan|GetSeconds (Math|Timespan|MakeTimespan 0 0 0 (Math|Float|Truncate (Variables|Default|GetCurrentLifeSpan)) 0)) false true 2 2)))))))))

(event Input|ActionEvents|InputActionInventory
  (params (Key :type Key%20Structure))
  (bind _pc_sky (Variables|Default|GetPC_Sky))
  (:Pressed
    (Utilities|IsValid (Variables|Default|GetW_CharDeadInsideInventory)
      (:Is%20Valid
        (Widget|RemovefromParent (Variables|Default|GetW_CharDeadInsideInventory))
        (Variables|Default|SetW_CharDeadInsideInventory 0) ; empty
        (Utilities|Platform|CollectGarbage))
      (:Is%20Not%20Valid
        (bind _returnvalue (UserInterface|CreateWidget "/Game/Widgets/W_CharDeadInsideInventory.W_CharDeadInsideInventory_C" _pc_sky _pc_sky self))
        (bind _output_get (Variables|Default|SetW_CharDeadInsideInventory _returnvalue))
        (UserInterface|Viewport|AddtoViewport _output_get 0)))))

(event Input|AxisEvents|InputAxisLookUp
  (params (AxisValue :type Float%20%28single-precision%29))
  (Variables|Default|SetLookRotation (Math|Rotator|MakeRotator (.roll (Variables|Default|GetLookRotation)) (Math|Float|ClampAngle (+ (* AxisValue -2.5) (.pitch (Variables|Default|GetLookRotation))) -9e+01 9e+01) (.yaw (Variables|Default|GetLookRotation)))))

(event Input|AxisEvents|InputAxisTurn
  (params (AxisValue :type Float%20%28single-precision%29))
  (Variables|Default|SetLookRotation (Math|Rotator|MakeRotator (.roll (Variables|Default|GetLookRotation)) (.pitch (Variables|Default|GetLookRotation)) (+ (* AxisValue 2.5) (.yaw (Variables|Default|GetLookRotation))))))

(event Input|KeyboardEvents|E
  (params (Key :type Key%20Structure))
  (:Pressed
    (Default|CreateWBSTransition (Variables|Default|GetPC_Sky) (delegate Custom|ShowBlackCompleted) self)
    (Input|DisableInput (Variables|Default|GetPC_Sky))))

(fn ConstructionScript)

(fn OnRepEssence
  (Default|CallEssenceChanged))

(fn ConsumeEssence
  (params (Essence :type S%20Essence%20Structure))
  (return false))

(fn GetACInventory
  (return (Variables|Default|GetAC_Inventory)))

(fn GetCharNormal
  (return 0))

(fn GetGeneratorIslands
  (return (Variables|Default|GetGenerator_Islands)))

(fn GetPCSky
  (return (Variables|Default|GetPC_Sky)))

(fn GetEssence
  (return (Variables|Default|GetEssence)))

(fn GetInteractionWidgetLocation
  (params (InteractionPlayer :type Pawn%20Object%20Reference))
  (return "0, 0, 0"))

(fn GetLookRotation
  (return (Variables|Default|GetLookRotation)))

(fn INT1Client
  (params (InteractedPawn :type Pawn%20Object%20Reference) (InteractedPC_Sky :type PC%20Sky%20Object%20Reference) (InteractedWith :type IC%20Class%20Reference))
  (bind _self self)
  (Default|EnableProlongedInteract (Variables|Default|GetAC_Interact) InteractedPawn InteractedPC_Sky)
  (bind _char_normal (Class|BPIGeneral|GetCharNormal(Message) InteractedPawn))
  (bind _returnvalue (UserInterface|CreateWidget "/Game/Widgets/CWS/CWS_CharDeadOutsideInventory.CWS_CharDeadOutsideInventory_C" InteractedPC_Sky _self _char_normal InteractedPC_Sky _self))
  (bind _output_get (Variables|Default|SetLOCAL_CWS_CharDeadOutsideInventory _returnvalue))
  (UserInterface|Viewport|AddtoViewport _output_get 0)
  (Default|AddCWS InteractedPC_Sky _output_get)
  (Default|SetMousetoCenter InteractedPC_Sky)
  (return true))

(fn INT1ClientInterrupt
  (params (InteractedPawn :type Pawn%20Object%20Reference) (InteractedPC_Sky :type PC%20Sky%20Object%20Reference) (InteractedWith :type IC%20Class%20Reference))
  (Default|RemoveCWS InteractedPC_Sky (Variables|Default|GetLOCAL_CWS_CharDeadOutsideInventory))
  (Variables|Default|SetLOCAL_CWS_CharDeadOutsideInventory 0) ; empty
  (return true))

(fn INT1Server
  (params (InteractedPawn :type Pawn%20Object%20Reference) (InteractedPC_Sky :type PC%20Sky%20Object%20Reference) (InteractedWith :type IC%20Class%20Reference))
  (return false))

(fn INT1ServerInterrupt
  (params (InteractedPawn :type Pawn%20Object%20Reference) (InteractedPC_Sky :type PC%20Sky%20Object%20Reference) (InteractedWith :type IC%20Class%20Reference))
  (return false))

(fn INT2Client
  (params (InteractedPawn :type Pawn%20Object%20Reference) (InteractedPC_Sky :type PC%20Sky%20Object%20Reference) (InteractedWith :type IC%20Class%20Reference))
  (return false))

(fn INT2ClientInterrupt
  (params (InteractedPawn :type Pawn%20Object%20Reference) (InteractedPC_Sky :type PC%20Sky%20Object%20Reference) (InteractedWith :type IC%20Class%20Reference))
  (return false))

(fn INT2Server
  (params (InteractedPawn :type Pawn%20Object%20Reference) (InteractedPC_Sky :type PC%20Sky%20Object%20Reference) (InteractedWith :type IC%20Class%20Reference))
  (bind _returnvalue (Transformation|GetActorRotation InteractedPawn))
  (bind _pc_sky (Variables|Default|GetPC_Sky))
  (bind _returnvalue_2 (Game|SpawnActorfromClass "/Game/Blueprints/SkyMain/Char_Normal.Char_Normal_C" (Math|Transform|MakeTransform (Transformation|GetActorLocation) (Math|Rotator|MakeRotator (.roll _returnvalue) (.pitch _returnvalue) (- (.yaw _returnvalue) 1.8e+02)) "1.000000,1.000000,1.000000") "AdjustIfPossibleButAlwaysSpawn" _pc_sky _pc_sky 0))
  (bind _output_get (Variables|/Game/Blueprints/SkyMain/PC_Sky.PC_Sky_C|SetChar_Normal (Variables|Default|GetPC_Sky) _returnvalue_2))
  (Variables|/Game/Blueprints/SkyMain/Char_Normal.Char_Normal_C|SetHealth _output_get 13.0)
  (Variables|/Game/Blueprints/SkyMain/Char_Normal.Char_Normal_C|SetHunger _returnvalue_2 13.0)
  (Default|MulticastInitSetup _returnvalue_2 (Variables|Default|GetEssence) (Variables|/Game/Inventory/AC_Inventory.AC_Inventory_C|GetInventory (Variables|Default|GetAC_Inventory)))
  (Rendering|SetActorHiddenInGame _returnvalue_2 false)
  (Pawn|Possess (Variables|Default|GetPC_Sky) _returnvalue_2)
  (Default|SpawnChunks (Variables|/Game/Blueprints/SkyMain/Char_Normal.Char_Normal_C|GetGenerator_Islands _returnvalue_2)) ; Force Spawn Chunks to avoid re-spawn
  (Default|MinusSpawnedChunks (Variables|Default|GetGenerator_Islands))
  (Default|SpawnChunks (Variables|/Game/Blueprints/SkyMain/Char_Normal.Char_Normal_C|GetGenerator_Essence _returnvalue_2)) ; Force Spawn Chunks to avoid re-spawn
  (Default|MinusSpawnedChunks (Variables|Default|GetGenerator_Essence))
  (CallFunction|ServerSideDestroyCharDead)
  (return true))

(fn INT2ServerInterrupt
  (params (InteractedPawn :type Pawn%20Object%20Reference) (InteractedPC_Sky :type PC%20Sky%20Object%20Reference) (InteractedWith :type IC%20Class%20Reference))
  (return false))

(fn INT3Client
  (params (InteractedPawn :type Pawn%20Object%20Reference) (InteractedPC_Sky :type PC%20Sky%20Object%20Reference) (InteractedWith :type IC%20Class%20Reference))
  (return false))

(fn INT3ClientInterrupt
  (params (InteractedPawn :type Pawn%20Object%20Reference) (InteractedPC_Sky :type PC%20Sky%20Object%20Reference) (InteractedWith :type IC%20Class%20Reference))
  (return false))

(fn INT3Server
  (params (InteractedPawn :type Pawn%20Object%20Reference) (InteractedPC_Sky :type PC%20Sky%20Object%20Reference) (InteractedWith :type IC%20Class%20Reference))
  (return false))

(fn INT3ServerInterrupt
  (params (InteractedPawn :type Pawn%20Object%20Reference) (InteractedPC_Sky :type PC%20Sky%20Object%20Reference) (InteractedWith :type IC%20Class%20Reference))
  (return false))

(fn SetEssence(Server)
  (params (Essence :type S%20Essence%20Structure))
  (bind _output_get (Variables|Default|SetEssence Essence))
  (return _output_get))

(fn SetLookRotation
  (params (LookRotation :type Rotator :default "0, 0, 0"))
  (return "0, 0, 0"))