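; Suffocation component that appears intended to suffocate a character who drops too far down, though the effect is unfinished.
; On BeginPlay the server enables ticking and caches the owner's CharNormal through a GetCharNormalMessage call.
; Tick tests whether that character is below a fixed world height, but the branch does nothing.
; A calculation based on MaxHealth is left unconnected.
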(event EventBeginPlay
  (if (Networking|IsServer)
    (Components|Tick|SetComponentTickEnabled true)
    (bind _char_normal (Class|BPIGeneral|GetCharNormal(Message) (Components|GetOwner)))
    (Variables|Default|SetChar_Normal _char_normal)))

(event EventTick
  (params (DeltaSeconds :type Float%20%28single-precision%29))
  (if (< (.z (Transformation|GetActorLocation (Variables|Default|GetChar_Normal))) -2e+04)
    _))