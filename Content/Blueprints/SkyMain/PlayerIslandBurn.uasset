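; Server-side component that burns a player island's Red, Green and Blue essence to pay for speed above normal.
; Each tick removes one unit of every selected color and deselects any that run out.
; UpdateTickBurnMatch sets the tick interval from selected color count over extra target speed, keeping total burn proportional to that excess.
; It disables ticking when the island stops or needs no boost, and resets speed to 1 when no color is selected.
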(event Custom|StopIslandChanged
  (CallFunction|UpdateTickBurnMatch))

(event EventBeginPlay
  (if (Networking|IsServer)
    (bind _playerisland (Class|BPIPlayerIsland|GetPlayerIsland(Message) (Components|GetOwner)))
    (bind _output_get (Variables|Default|SetPlayerIsland _playerisland))
    (EventDispatchers|BindEventtoStopIslandChanged _output_get (delegate Custom|StopIslandChanged))))

(event EventTick
  (params (DeltaSeconds :type Float%20%28single-precision%29))
  (bind _playerisland (Variables|Default|GetPlayerIsland))
  (bind _playerisland_2 (Variables|Default|GetPlayerIsland))
  (bind _playerisland_3 (Variables|Default|GetPlayerIsland))
  (Utilities|FlowControl|Sequence
    (:then_0
      (Variables|Default|SetTempEssence (Variables|/Game/Blueprints/SkyMain/PlayerIsland.PlayerIsland_C|GetEssence (Variables|Default|GetPlayerIsland)))
      (Utilities|FlowControl|Sequence
        (:then_0
          (if (.red (Variables|/Game/Blueprints/SkyMain/PlayerIsland.PlayerIsland_C|GetEssenceBurnSelect (Variables|Default|GetPlayerIsland))) ; Burn Red Slected?
            (if (> (.red (Variables|Default|GetTempEssence)) 0) ; Red > 0
              (Variables|Default|SetTempEssence (Utilities|Struct|MakeS_Essence (- (.red (Variables|Default|GetTempEssence)) 1) (.green (Variables|Default|GetTempEssence)) (.blue (Variables|Default|GetTempEssence)))) ; Burn 1 Red
            )
            (if (not (> (.red (Variables|Default|GetTempEssence)) 0)) ; Red > 0
              (Variables|/Game/Blueprints/SkyMain/PlayerIsland.PlayerIsland_C|SetEssenceBurnSelect _playerisland (Utilities|Struct|MakeS_EssenceSelect false (.green (Variables|/Game/Blueprints/SkyMain/PlayerIsland.PlayerIsland_C|GetEssenceBurnSelect _playerisland)) (.blue (Variables|/Game/Blueprints/SkyMain/PlayerIsland.PlayerIsland_C|GetEssenceBurnSelect _playerisland)))) ; Disable Red
              (CallFunction|UpdateTickBurnMatch))))
        (:then_1
          (if (.green (Variables|/Game/Blueprints/SkyMain/PlayerIsland.PlayerIsland_C|GetEssenceBurnSelect (Variables|Default|GetPlayerIsland)))
            (if (> (.green (Variables|Default|GetTempEssence)) 0) ; Green > 0
              (Variables|Default|SetTempEssence (Utilities|Struct|MakeS_Essence (.red (Variables|Default|GetTempEssence)) (- (.green (Variables|Default|GetTempEssence)) 1) (.blue (Variables|Default|GetTempEssence)))) ; Burn 1 Green
            )
            (if (not (> (.green (Variables|Default|GetTempEssence)) 0)) ; Green > 0
              (Variables|/Game/Blueprints/SkyMain/PlayerIsland.PlayerIsland_C|SetEssenceBurnSelect _playerisland_2 (Utilities|Struct|MakeS_EssenceSelect (.red (Variables|/Game/Blueprints/SkyMain/PlayerIsland.PlayerIsland_C|GetEssenceBurnSelect _playerisland_2)) false (.blue (Variables|/Game/Blueprints/SkyMain/PlayerIsland.PlayerIsland_C|GetEssenceBurnSelect _playerisland_2)))) ; Disable Green
              (CallFunction|UpdateTickBurnMatch))))
        (:then_2
          (if (.blue (Variables|/Game/Blueprints/SkyMain/PlayerIsland.PlayerIsland_C|GetEssenceBurnSelect (Variables|Default|GetPlayerIsland)))
            (if (> (.blue (Variables|Default|GetTempEssence)) 0) ; Blue > 0
              (Variables|Default|SetTempEssence (Utilities|Struct|MakeS_Essence (.red (Variables|Default|GetTempEssence)) (.green (Variables|Default|GetTempEssence)) (- (.blue (Variables|Default|GetTempEssence)) 1))) ; Burn 1 Blue
            )
            (if (not (> (.blue (Variables|Default|GetTempEssence)) 0)) ; Blue > 0
              (Variables|/Game/Blueprints/SkyMain/PlayerIsland.PlayerIsland_C|SetEssenceBurnSelect _playerisland_3 (Utilities|Struct|MakeS_EssenceSelect (.red (Variables|/Game/Blueprints/SkyMain/PlayerIsland.PlayerIsland_C|GetEssenceBurnSelect _playerisland_3)) (.green (Variables|/Game/Blueprints/SkyMain/PlayerIsland.PlayerIsland_C|GetEssenceBurnSelect _playerisland_3)) false)) ; Diisable Blue
              (CallFunction|UpdateTickBurnMatch))))))
    (:then_1
      (Variables|/Game/Blueprints/SkyMain/PlayerIsland.PlayerIsland_C|SetEssence (Variables|Default|GetPlayerIsland) (Variables|Default|GetTempEssence)))))

(fn UpdateTickBurnMatch
  (bind _playerisland (Variables|Default|GetPlayerIsland))
  (bind _essenceburnselect (Variables|/Game/Blueprints/SkyMain/PlayerIsland.PlayerIsland_C|GetEssenceBurnSelect _playerisland))
  (if (Variables|/Game/Blueprints/SkyMain/PlayerIsland.PlayerIsland_C|GetStopIsland (Variables|Default|GetPlayerIsland))
    (Components|Tick|SetComponentTickEnabled false)
    (elif (> (Variables|/Game/Blueprints/SkyMain/PlayerIsland.PlayerIsland_C|GetTargetSpeed (Variables|Default|GetPlayerIsland)) 1.0)
      (Utilities|FlowControl|Sequence
        (:then_0
          (if (.red _essenceburnselect)
            (LocalVariables|SetEssenceSelectNum (+ 1 (LocalVariables|GetEssenceSelectNum)) :!label _label)))
        (:then_1
          (if (.green _essenceburnselect)
            (goto _label)))
        (:then_2
          (if (.blue _essenceburnselect)
            (goto _label)))
        (:then_3
          (if (> (LocalVariables|GetEssenceSelectNum) 0)
            (Class|ActorComponent|SetComponentTickInterval (/ (LocalVariables|GetEssenceSelectNum) (- (Variables|/Game/Blueprints/SkyMain/PlayerIsland.PlayerIsland_C|GetTargetSpeed (Variables|Default|GetPlayerIsland)) 1.0)))
            (Components|Tick|SetComponentTickEnabled true)
            (else
              (Variables|/Game/Blueprints/SkyMain/PlayerIsland.PlayerIsland_C|SetTargetSpeed (Variables|Default|GetPlayerIsland) 1.0)
              (Components|Tick|SetComponentTickEnabled false)))))
      (else
        (Components|Tick|SetComponentTickEnabled false)))))