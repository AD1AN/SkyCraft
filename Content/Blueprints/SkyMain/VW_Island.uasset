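; VW_Island is a voxel world actor for an island generated from replicated chunk data.
; On BeginPlay it announces itself as initialized through the game instance's SGI message object.
; When Chunk replicates, its RepNotify picks a server or client spawner config, passes the chunk's seed and scale to the generator, then creates the world.
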(event EventBeginPlay
  (bind _sgi (Class|BPISGI|GetSGI(Message) (Game|GetGameInstance)))
  (bind _output_get (Variables|Default|SetSGI _sgi))
  (Default|CallIslandInitialized _output_get self))

(fn ConstructionScript)

(fn OnRepChunk
  (bind _chunk (Variables|Default|GetChunk))
  (if (Networking|IsServer)
    (Variables|Default|SetSpawnerConfig "/Game/Blueprints/SkyMain/SC_Server.SC_Server")
    (else
      (Variables|Default|SetSpawnerConfig "/Game/Blueprints/SkyMain/SC_Client.SC_Client")))
  (Class|VoxelGeneratorTools|SetGeneratorParameter (Variables|Default|GetGenerator) "SeedName" (Variables|/Game/Blueprints/SkyMain/SA_Chunk_Islands.SA_Chunk_Islands_C|GetChunkSeed _chunk))
  (Class|VoxelGeneratorTools|SetGeneratorParameter (Variables|Default|GetGenerator) "Scale" (Variables|/Game/Blueprints/SkyMain/SA_Chunk_Islands.SA_Chunk_Islands_C|GetChunkScale _chunk))
  (Class|VoxelWorld|CreateWorld self))