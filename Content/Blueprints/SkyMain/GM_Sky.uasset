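; GM_Sky is the game mode for the Sky world, handling player join and logout, chat broadcast, client disconnection and world persistence.
; On first start it caches the game instance, game state and PlayerIsland, then loads or creates the WorldName save slot.
; SaveGame snapshots buildings, island, players, corpses and item drops, storing island-attached transforms relatively for buildings and players.
; Logout saves that player by PlayerID; LastSave blocks writes after the exit save.
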(event Custom|SendMessageToEveryone
  (params (Sender :type String) (Message :type String))
  (for _array_element (Variables|/Game/Blueprints/SGI.SGI_C|GetPlayers (Variables|Default|GetSGI))
    (Default|AddMessagetoChat _array_element Sender Message)))

(event Custom|CustomBeginPlay
  (Variables|Default|SethadBeginPlayer true)
  (bind _sgi (Class|BPISGI|GetSGI(Message) (Game|GetGameInstance)))
  (bind _output_get (Variables|Default|SetSGI _sgi))
  (Variables|/Game/Blueprints/SGI.SGI_C|SetGM_Sky _output_get self)
  (bind _gs_sky (Class|BPIGameMS|GetGSSky(Message) (Game|GetGameState)))
  (Variables|Default|SetGS_Sky _gs_sky)
  (bind _returnvalue (Actor|GetActorOfClass "/Game/Blueprints/SkyMain/PlayerIsland.PlayerIsland_C"))
  (Variables|Default|SetPlayerIsland _returnvalue)
  (bind _output_get_2 (Variables|Default|SetWorldName (Variables|/Game/Blueprints/SGI.SGI_C|GetWorldName (Variables|Default|GetSGI))))
  (bind _returnvalue_2 (SaveGame|DoesSaveGameExist _output_get_2))
  (if _returnvalue_2
    (CallFunction|LoadGame)
    (else
      (bind _returnvalue_3 (SaveGame|CreateSaveGameObject "/Game/Blueprints/SSG.SSG_C"))
      (SaveGame|SaveGametoSlot _returnvalue_3 (Variables|Default|GetWorldName)))))

(event Custom|DisconnectAllClients
  (for _array_element (Variables|/Game/Blueprints/SGI.SGI_C|GetPlayers (Variables|Default|GetSGI))
    (Default|ClientDisconnect _array_element)))

(event Custom|PlayerIslandCollision
  (bind _playerisland (Variables|Default|GetPlayerIsland))
  (Default|ServerStopPlayerIsland (Variables|Default|GetPlayerIsland))
  (Variables|/Game/Blueprints/SkyMain/PlayerIsland.PlayerIsland_C|SetCurrentDirection _playerisland "0, 0, 0")
  (Transformation|SetActorLocation (Variables|/Game/Blueprints/SkyMain/PlayerIsland.PlayerIsland_C|GetPreviousLocation _playerisland) false false))

(event EventBeginPlay
  (if (not (Variables|Default|GethadBeginPlayer))
    (CallFunction|CustomBeginPlay)))

(event EventOnLogout
  (params (ExitingController :type Controller%20Object%20Reference))
  (Variables|Default|SetTestNameClient (- (Variables|Default|GetTestNameClient) 1))
  (bind _aspc_sky (Utilities|Casting|CastToPC_Sky ExitingController))
  (Utilities|Array|RemoveItem (Variables|/Game/Blueprints/SGI.SGI_C|GetPlayers (Variables|Default|GetSGI)) _aspc_sky)
  (bind _returnvalue (SaveGame|DoesSaveGameExist (Variables|Default|GetWorldName)))
  (if _returnvalue
    (bind _returnvalue_2 (SaveGame|LoadGamefromSlot (Variables|Default|GetWorldName)))
    (bind _ssg (Class|BPISSG|GetSSG(Message) _returnvalue_2))
    (CallFunction|SavePlayer _ssg _aspc_sky))
  (if (not (Variables|Default|GetLastSave))
    (switch Utilities|FlowControl|Switch|SwitchonPlayerForm (Variables|/Game/Blueprints/SkyMain/PC_Sky.PC_Sky_C|GetPlayerForm _aspc_sky)
      (:NewEnumerator0
        (Actor|DestroyActor (Variables|/Game/Blueprints/SkyMain/PC_Sky.PC_Sky_C|GetChar_Island _aspc_sky)))
      (:NewEnumerator2
        (Utilities|IsValid (Variables|/Game/Blueprints/SkyMain/Char_Normal.Char_Normal_C|GetChar_Spirit (Variables|/Game/Blueprints/SkyMain/PC_Sky.PC_Sky_C|GetChar_Normal _aspc_sky))
          (:Is%20Valid
            (Actor|DestroyActor (Variables|/Game/Blueprints/SkyMain/Char_Normal.Char_Normal_C|GetChar_Spirit (Variables|/Game/Blueprints/SkyMain/PC_Sky.PC_Sky_C|GetChar_Normal _aspc_sky))))
          (:Is%20Not%20Valid
            _))
        (Actor|DestroyActor (Variables|/Game/Blueprints/SkyMain/PC_Sky.PC_Sky_C|GetChar_Normal _aspc_sky)))
      (:NewEnumerator3
        (Actor|DestroyActor (Variables|/Game/Blueprints/SkyMain/Char_Normal.Char_Normal_C|GetChar_Spirit (Variables|/Game/Blueprints/SkyMain/PC_Sky.PC_Sky_C|GetChar_Normal _aspc_sky)))
        (Actor|DestroyActor (Variables|/Game/Blueprints/SkyMain/PC_Sky.PC_Sky_C|GetChar_Normal _aspc_sky)))
      (:NewEnumerator1
        (Actor|DestroyActor (Variables|/Game/Blueprints/SkyMain/PC_Sky.PC_Sky_C|GetChar_Dead _aspc_sky))))))

(event EventPostLogin
  (params (NewPlayer :type Player%20Controller%20Object%20Reference)))

(event EventHandleStartingNewPlayer
  (params (NewPlayer :type Player%20Controller%20Object%20Reference))
  (if (Variables|Default|GethadBeginPlayer)
    _
    (else
      (CallFunction|CustomBeginPlay)))
  (bind _aspc_sky (Utilities|Casting|CastToPC_Sky NewPlayer))
  (Variables|/Game/Blueprints/SkyMain/PC_Sky.PC_Sky_C|SetPlayerIsland _aspc_sky (Variables|Default|GetPlayerIsland))
  (Utilities|Array|Add (Variables|/Game/Blueprints/SGI.SGI_C|GetPlayers (Variables|Default|GetSGI)) _aspc_sky))

(fn ConstructionScript)

(fn SaveGame
  (params (LastExitSave? :type Boolean))
  (bind _playerisland (Variables|Default|GetPlayerIsland))
  (if (not (Variables|Default|GetLastSave))
    (bind _returnvalue (SaveGame|DoesSaveGameExist (Variables|Default|GetWorldName)))
    (if _returnvalue
      (bind _returnvalue_2 (SaveGame|LoadGamefromSlot (Variables|Default|GetWorldName)))
      (bind _ssg (Class|BPISSG|GetSSG(Message) _returnvalue_2))
      (LocalVariables|Set_SSG _ssg)
      (else
        (bind _returnvalue_3 (SaveGame|CreateSaveGameObject "/Game/Blueprints/SSG.SSG_C"))
        (LocalVariables|Set_SSG _returnvalue_3)))
    (Variables|/Game/Blueprints/SSG.SSG_C|SetLastPlayed (LocalVariables|Get_SSG) (Math|DateTime|Now))
    (Utilities|FlowControl|Sequence
      (:then_0
        ;[1 0.2892 0.1795 1 55] Building Actors
        (Utilities|Array|Clear (Variables|/Game/Blueprints/SSG.SSG_C|GetSSG_BuildingActor (LocalVariables|Get_SSG)))
        (bind _outactors (Actor|GetAllActorsOfClass "/Game/Building/BuildingActor.BuildingActor_C"))
        (for _array_element _outactors
          (if (== (Components|GetOwner _array_element) 0) ; Check if this build not in Preview
            (Utilities|Array|Add (Variables|/Game/Blueprints/SSG.SSG_C|GetSSG_BuildingActor (LocalVariables|Get_SSG)) (Utilities|Struct|MakeSSG_BuildingActor (Utilities|GetClass _array_element) (not (== (Actor|GetAttachParentActor _array_element) 0)) (Math|Transform|SelectTransform (Transformation|GetRelativeTransform (Variables|/Game/Building/BuildingActor.BuildingActor_C|GetScene _array_element)) (Transformation|GetActorTransform _array_element) (not (== (Actor|GetAttachParentActor _array_element) 0))) (Variables|/Game/Building/BuildingActor.BuildingActor_C|GetCurrentHealth _array_element) (Variables|/Game/Building/BuildingActor.BuildingActor_C|GetMaxHealth _array_element))))))
      (:then_1
        ;[0.5141 1 0.5219 1 55] Player Island
        (Variables|/Game/Blueprints/SSG.SSG_C|SetSSG_PlayerIsland (LocalVariables|Get_SSG) (Utilities|Struct|MakeSSG_PlayerIsland (Transformation|GetActorTransform _playerisland) (Variables|/Game/Blueprints/SkyMain/PlayerIsland.PlayerIsland_C|GetTargetDirection _playerisland) (Variables|/Game/Blueprints/SkyMain/PlayerIsland.PlayerIsland_C|GetTargetAltitude _playerisland) (Variables|/Game/Blueprints/SkyMain/PlayerIsland.PlayerIsland_C|GetTargetSpeed _playerisland) (Variables|/Game/Blueprints/SkyMain/PlayerIsland.PlayerIsland_C|GetStopIsland _playerisland) (Variables|/Game/Blueprints/SkyMain/PlayerIsland.PlayerIsland_C|GetEssence _playerisland) (Variables|/Game/Blueprints/SkyMain/PlayerIsland.PlayerIsland_C|GetEssenceBurnSelect _playerisland))))
      (:then_2
        ;[0.05432 0.3611 1 1 55] Players
        (for _array_element_2 (Variables|/Game/Blueprints/SGI.SGI_C|GetPlayers (Variables|Default|GetSGI))
          (bind _output_get (LocalVariables|Set_ElementPC_Sky _array_element_2))
          (CallFunction|SavePlayer (LocalVariables|Get_SSG) _output_get)))
      (:then_3
        ;[0.2926 0.3021 0.2832 1 55] Char Dead
        (Utilities|Array|Clear (Variables|/Game/Blueprints/SSG.SSG_C|GetSSG_Char_Dead (LocalVariables|Get_SSG)))
        (bind _outactors_2 (Actor|GetAllActorsOfClass "/Game/Blueprints/SkyMain/Char_Dead.Char_Dead_C"))
        (for _array_element_3 _outactors_2
          (Utilities|IsValid (Variables|/Game/Blueprints/SkyMain/Char_Dead.Char_Dead_C|GetPC_Sky _array_element_3)
            (:Is%20Not%20Valid
              (Utilities|Array|Add (Variables|/Game/Blueprints/SSG.SSG_C|GetSSG_Char_Dead (LocalVariables|Get_SSG)) (Utilities|Struct|MakeSSG_Char_Dead (Transformation|GetActorLocation _array_element_3) (Variables|/Game/Blueprints/SkyMain/Char_Dead.Char_Dead_C|GetEssence _array_element_3) (Variables|/Game/Inventory/AC_Inventory.AC_Inventory_C|GetInventory (Variables|/Game/Blueprints/SkyMain/Char_Dead.Char_Dead_C|GetAC_Inventory _array_element_3)) (Variables|/Game/Blueprints/SkyMain/Char_Dead.Char_Dead_C|GetCurrentLifeSpan _array_element_3)))))))
      (:then_4
        ;[0.6042 1 0.952 1 55] Item Drop
        (Utilities|Array|Clear (Variables|/Game/Blueprints/SSG.SSG_C|GetSSG_ItemDrop (LocalVariables|Get_SSG)))
        (bind _outactors_3 (Actor|GetAllActorsOfClass "/Game/Inventory/ItemDrop.ItemDrop_C"))
        (for _array_element_4 _outactors_3
          (Utilities|Array|Add (Variables|/Game/Blueprints/SSG.SSG_C|GetSSG_ItemDrop (LocalVariables|Get_SSG)) (Utilities|Struct|MakeSSG_ItemDrop (Transformation|GetActorLocation _array_element_4) (Utilities|IsValid (Actor|GetAttachParentActor _array_element_4)) (Physics|IsSimulatingPhysics (Variables|/Game/Inventory/ItemDrop.ItemDrop_C|GetStaticMesh _array_element_4) "None") (Variables|/Game/Inventory/AC_Inventory.AC_Inventory_C|GetInventory (Variables|/Game/Inventory/ItemDrop.ItemDrop_C|GetAC_Inventory _array_element_4)) (Actor|GetLifeSpan _array_element_4)))))
      (:then_5
        ;[1 0.09423 0.994 1 40] End save
        (SaveGame|SaveGametoSlot (LocalVariables|Get_SSG) (Variables|Default|GetWorldName))
        (Variables|Default|SetLastSave LastExitSave?)))))

(fn LoadGame
  (bind _returnvalue (SaveGame|LoadGamefromSlot (Variables|Default|GetWorldName)))
  (bind _ssg (Class|BPISSG|GetSSG(Message) _returnvalue))
  (bind _output_get (LocalVariables|Set_SSG _ssg))
  (Variables|Default|SetWorldSeed (Variables|/Game/Blueprints/SSG.SSG_C|GetWorldSeed _output_get))
  (Utilities|FlowControl|Sequence
    (:then_0
      (for _array_element (Variables|/Game/Blueprints/SSG.SSG_C|GetSSG_BuildingActor (LocalVariables|Get_SSG))
        (bind _returnvalue_2 (Game|SpawnActorfromClass :Class (.BuildingClass (Utilities|Struct|BreakSSG_BuildingActor _array_element)) :SpawnTransform (.Transform (Utilities|Struct|BreakSSG_BuildingActor _array_element)) :CollisionHandlingOverride "AlwaysSpawn" :Instigator 0))
        (if (.AttachedToPI (Utilities|Struct|BreakSSG_BuildingActor _array_element))
          (Transformation|AttachActorToActor _returnvalue_2 (Variables|Default|GetPlayerIsland) "None" "KeepRelative" "KeepRelative" "KeepRelative" true))
        (Variables|/Game/Building/BuildingActor.BuildingActor_C|SetCurrentHealth _returnvalue_2 (.CurrentHealth (Utilities|Struct|BreakSSG_BuildingActor _array_element)))
        (Variables|/Game/Building/BuildingActor.BuildingActor_C|SetMaxHealth _returnvalue_2 (.MaxHealth (Utilities|Struct|BreakSSG_BuildingActor _array_element)))))
    (:then_1
      (Variables|Default|SetPlayerIslandLoadedFromSave true)
      (Transformation|SetActorTransform (Variables|Default|GetPlayerIsland) (.Transform (Utilities|Struct|BreakSSG_PlayerIsland (Variables|/Game/Blueprints/SSG.SSG_C|GetSSG_PlayerIsland (LocalVariables|Get_SSG)))) false true)
      (|PlayerIslandSet (.TargetDirection (Utilities|Struct|BreakSSG_PlayerIsland (Variables|/Game/Blueprints/SSG.SSG_C|GetSSG_PlayerIsland (LocalVariables|Get_SSG)))) (.TargetAltitude (Utilities|Struct|BreakSSG_PlayerIsland (Variables|/Game/Blueprints/SSG.SSG_C|GetSSG_PlayerIsland (LocalVariables|Get_SSG)))) (.TargetSpeed (Utilities|Struct|BreakSSG_PlayerIsland (Variables|/Game/Blueprints/SSG.SSG_C|GetSSG_PlayerIsland (LocalVariables|Get_SSG)))) (.StopIsland (Utilities|Struct|BreakSSG_PlayerIsland (Variables|/Game/Blueprints/SSG.SSG_C|GetSSG_PlayerIsland (LocalVariables|Get_SSG)))) (.Essence (Utilities|Struct|BreakSSG_PlayerIsland (Variables|/Game/Blueprints/SSG.SSG_C|GetSSG_PlayerIsland (LocalVariables|Get_SSG)))) (.EssenceBurnSelect (Utilities|Struct|BreakSSG_PlayerIsland (Variables|/Game/Blueprints/SSG.SSG_C|GetSSG_PlayerIsland (LocalVariables|Get_SSG)))))
      (Variables|/Game/Blueprints/SkyMain/PlayerIslandBurn.PlayerIslandBurn_C|SetPlayerIsland (Variables|/Game/Blueprints/SkyMain/PlayerIsland.PlayerIsland_C|GetPlayerIslandBurn (Variables|Default|GetPlayerIsland)) (Variables|Default|GetPlayerIsland))
      (Default|UpdateTickBurnMatch (Variables|/Game/Blueprints/SkyMain/PlayerIsland.PlayerIsland_C|GetPlayerIslandBurn (Variables|Default|GetPlayerIsland))))
    (:then_2
      (Utilities|FlowControl|Sequence
        (:then_0
          (for _array_element_2 (Variables|/Game/Blueprints/SSG.SSG_C|GetSSG_Char_Dead (LocalVariables|Get_SSG))
            (bind _returnvalue_3 (Game|SpawnActorfromClass "/Game/Blueprints/SkyMain/Char_Dead.Char_Dead_C" (Math|Transform|MakeTransform (.Location (Utilities|Struct|BreakSSG_Char_Dead _array_element_2)) "0, 0, 0" "1.000000,1.000000,1.000000") "AlwaysSpawn" 0 0 0 0))
            (Variables|/Game/Blueprints/SkyMain/Char_Dead.Char_Dead_C|SetEssence _returnvalue_3 (.Essence (Utilities|Struct|BreakSSG_Char_Dead _array_element_2)))
            (Variables|/Game/Inventory/AC_Inventory.AC_Inventory_C|SetInventory (Variables|/Game/Blueprints/SkyMain/Char_Dead.Char_Dead_C|GetAC_Inventory _returnvalue_3) (.Inventory (Utilities|Struct|BreakSSG_Char_Dead _array_element_2)))
            (Variables|/Game/Blueprints/SkyMain/Char_Dead.Char_Dead_C|SetCurrentLifeSpan _returnvalue_3 (.CurrentLifeSpan (Utilities|Struct|BreakSSG_Char_Dead _array_element_2)))))
        (:then_1
          (for _array_element_3 (Variables|/Game/Blueprints/SSG.SSG_C|GetSSG_ItemDrop (LocalVariables|Get_SSG))
            (bind _returnvalue_4 (Game|SpawnActorfromClass "/Game/Inventory/ItemDrop.ItemDrop_C" (Math|Transform|MakeTransform (.Location (Utilities|Struct|BreakSSG_ItemDrop _array_element_3)) "0, 0, 0" "1.000000,1.000000,1.000000") "AlwaysSpawn" 0 0))
            (if (.AttachedToPI (Utilities|Struct|BreakSSG_ItemDrop _array_element_3))
              (Transformation|AttachActorToActor _returnvalue_4 (Variables|Default|GetPlayerIsland) "None" "KeepWorld" "KeepWorld" "KeepWorld" true))
            (Physics|SetSimulatePhysics (Variables|/Game/Inventory/ItemDrop.ItemDrop_C|GetStaticMesh _returnvalue_4) (.SimulatePhysics (Utilities|Struct|BreakSSG_ItemDrop _array_element_3)))
            (if (not (.SimulatePhysics (Utilities|Struct|BreakSSG_ItemDrop _array_element_3)))
              (Default|StartIdle _returnvalue_4))
            (Actor|SetLifeSpan _returnvalue_4 (.RemainLifeSpan (Utilities|Struct|BreakSSG_ItemDrop _array_element_3)))
            (Variables|/Game/Inventory/AC_Inventory.AC_Inventory_C|SetInventory (Variables|/Game/Inventory/ItemDrop.ItemDrop_C|GetAC_Inventory _returnvalue_4) (.Inventory (Utilities|Struct|BreakSSG_ItemDrop _array_element_3)))))))))

(fn SavePlayer
  (params (_SSG :type SSG%20Object%20Reference) (_ElementPC_Sky :type PC%20Sky%20Object%20Reference))
  (bind _char_normal (Variables|/Game/Blueprints/SkyMain/PC_Sky.PC_Sky_C|GetChar_Normal _ElementPC_Sky))
  (bind _char_normal_2 (Variables|/Game/Blueprints/SkyMain/PC_Sky.PC_Sky_C|GetChar_Normal _ElementPC_Sky))
  (bind _char_island (Variables|/Game/Blueprints/SkyMain/PC_Sky.PC_Sky_C|GetChar_Island _ElementPC_Sky))
  (bind _char_dead (Variables|/Game/Blueprints/SkyMain/PC_Sky.PC_Sky_C|GetChar_Dead _ElementPC_Sky))
  (bind _playerform (Variables|/Game/Blueprints/SkyMain/PC_Sky.PC_Sky_C|GetPlayerForm _ElementPC_Sky))
  (bind _char_normal_3 (Variables|/Game/Blueprints/SkyMain/PC_Sky.PC_Sky_C|GetChar_Normal _ElementPC_Sky))
  (bind _returnvalue (Utilities|Select :Index _playerform :NewEnumerator0 _char_island :NewEnumerator2 _char_normal_2 :NewEnumerator3 _char_normal_2 :NewEnumerator1 _char_dead))
  (bind _attachedtopi (Variables|/Game/Blueprints/SkyMain/Char_Normal.Char_Normal_C|GetAttachedToPI _char_normal))
  (bind _char_spirit (Variables|/Game/Blueprints/SkyMain/Char_Normal.Char_Normal_C|GetChar_Spirit _char_normal_3))
  (if (not (Variables|Default|GetLastSave))
    (Utilities|Struct|SetmembersinSSG_Player (LocalVariables|Get_SavingPlayer) (Transformation|GetActorTransform _returnvalue))
    (bind _lookrotation (Class|BPIChars|GetLookRotation(Message) _returnvalue))
    (bind _essence (Class|BPIEssence|GetEssence(Message) _returnvalue))
    (bind _ac_inventory (Class|BPIGeneral|GetACInventory(Message) _returnvalue))
    (Utilities|IsValid (Variables|/Game/Blueprints/SkyMain/PC_Sky.PC_Sky_C|GetChar_Normal _ElementPC_Sky)
      (:Is%20Valid
        (Utilities|Struct|SetmembersinSSG_Player (LocalVariables|Get_SavingPlayer) _attachedtopi (Math|Transform|SelectTransform (Math|Transform|MakeTransform (Math|Transform|InverseTransformLocation (Transformation|GetActorTransform (Variables|Default|GetPlayerIsland)) (Transformation|GetActorLocation _char_normal)) (Transformation|GetActorRotation _char_normal) "1.000000,1.000000,1.000000") (Transformation|GetActorTransform _char_normal) _attachedtopi) (Utilities|IsValid (Variables|/Game/Blueprints/SkyMain/Char_Normal.Char_Normal_C|GetChar_Spirit _char_normal)))
        (Utilities|IsValid _char_spirit
          (:Is%20Valid
            (Utilities|Struct|SetmembersinSSG_Player (LocalVariables|Get_SavingPlayer) (Transformation|GetActorLocation _char_spirit) (Variables|/Game/Blueprints/SkyMain/Char_Spirit.Char_Spirit_C|GetLookRotation _char_spirit)))
          (:Is%20Not%20Valid
            _)))
      (:Is%20Not%20Valid
        _))
    (Utilities|Struct|SetmembersinSSG_Player (LocalVariables|Get_SavingPlayer) (Variables|/Game/Blueprints/SkyMain/PC_Sky.PC_Sky_C|GetPlayerID _ElementPC_Sky) (Variables|/Game/Blueprints/SkyMain/PC_Sky.PC_Sky_C|GetPlayerForm _ElementPC_Sky) _lookrotation _essence (Utilities|Select :Index (Variables|/Game/Blueprints/SkyMain/PC_Sky.PC_Sky_C|GetPlayerForm _ElementPC_Sky) :NewEnumerator0 0 :NewEnumerator2 (Variables|/Game/Blueprints/SkyMain/PC_Sky.PC_Sky_C|GetActiveQSI _ElementPC_Sky) :NewEnumerator3 (Variables|/Game/Blueprints/SkyMain/PC_Sky.PC_Sky_C|GetPrevQSI _ElementPC_Sky) :NewEnumerator1 0) (Variables|/Game/Inventory/AC_Inventory.AC_Inventory_C|GetInventory _ac_inventory))
    (Utilities|FlowControl|Sequence
      (:then_0
        (for (_array_element _array_index) (Variables|/Game/Blueprints/SSG.SSG_C|GetSSG_Player _SSG)
          (if (Utilities|Enum|Equal(Enum) (Utilities|Struct|BreakSSG_Player _array_element) (Variables|/Game/Blueprints/SkyMain/PC_Sky.PC_Sky_C|GetPlayerID _ElementPC_Sky))
            (LocalVariables|Set_SavingPlayerFound true)
            (Utilities|Array|SetArrayElem (Variables|/Game/Blueprints/SSG.SSG_C|GetSSG_Player _SSG) _array_index (LocalVariables|Get_SavingPlayer))))
        (if (not (LocalVariables|Get_SavingPlayerFound))
          (Utilities|Array|Add (Variables|/Game/Blueprints/SSG.SSG_C|GetSSG_Player _SSG) (LocalVariables|Get_SavingPlayer))))
      (:then_1
        (SaveGame|SaveGametoSlot _SSG (Variables|Default|GetWorldName))))))

(fn GetGMSky
  (return self))

(fn GetGSSky
  (return 0))