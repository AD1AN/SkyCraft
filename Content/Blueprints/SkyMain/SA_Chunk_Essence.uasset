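; SA_Chunk_Essence is a world chunk actor that populates its box with Essence pickups and LootCrystals.
; On BeginPlay the server runs four alternating passes of delayed loops, spawning both at random points inside ChunkBox.
; Essences roll weighted red, green or blue-dominant values, while crystals get mixed essence and random Wood or Stone inventory.
; When replicated HMPR drops to zero, DestroyChunk unregisters it from GMSky, destroys its spawned actors, then itself.
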(event EventBeginPlay
  (if (Networking|IsServer)
    (Utilities|LOOPEssence
      (:Completed
        (Utilities|LOOPLootCrystal
          (:Completed
            (Utilities|LOOPEssence
              (:Completed
                (Utilities|LOOPLootCrystal
                  (:Completed
                    (Utilities|LOOPEssence
                      (:Completed
                        (Utilities|LOOPLootCrystal
                          (:Completed
                            (Utilities|LOOPEssence
                              (:Completed
                                (Utilities|LOOPLootCrystal)))))))))))))))))

(fn ConstructionScript)

(fn DestroyChunk
  (bind _self self)
  (bind _gm_sky (Variables|Default|GetGM_Sky))
  (bind _gm_sky_2 (Variables|Default|GetGM_Sky))
  (bind _spawnedchunkessence (Variables|/Game/Blueprints/SkyMain/GM_Sky.GM_Sky_C|GetSpawnedChunkEssence _gm_sky_2))
  (bind _returnvalue (Utilities|Array|FindItem _spawnedchunkessence _self))
  (Utilities|Array|RemoveIndex (Variables|/Game/Blueprints/SkyMain/GM_Sky.GM_Sky_C|GetSpawnedChunkEssenceCors _gm_sky) _returnvalue)
  (Utilities|Array|RemoveIndex (Variables|/Game/Blueprints/SkyMain/GM_Sky.GM_Sky_C|GetSpawnedChunkEssence _gm_sky) _returnvalue)
  (Utilities|FlowControl|Sequence
    (:then_0
      (for _array_element (Variables|Default|GetEssences)
        (Utilities|IsValid _array_element
          (:Is%20Valid
            (Default|DestroyEssence _array_element))))
      (for _array_element_2 (Variables|Default|GetLootCrystals)
        (Utilities|IsValid _array_element_2
          (:Is%20Valid
            (Default|DestroyLootCrystal _array_element_2)))))
    (:then_1
      (Actor|DestroyActor))))

(fn OnRepHMPR
  (if (<= (Variables|Default|GetHMPR) 0)
    (CallFunction|DestroyChunk)))