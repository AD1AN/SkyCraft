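; Player-possessed flying cinematic camera character with a toggleable HUD and settings widget, able to spawn or delete PF_Normal characters where it looks.
; Input drives a look rotation applied to a spring arm and used for movement direction.
; The mouse wheel with held keys tunes fly speed, sensitivity or arm length, with Shift as a boost.
; Look rotation replicates via unreliable server-to-multicast calls; fly speed syncs to the server.
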(event Custom|Server_ChangeFlySpeed
  (params (Max%20Fly%20Speed :type Float%20%28single-precision%29))
  (Variables|/Script/Engine.CharacterMovementComponent|SetMaxFlySpeed (Variables|Character|GetCharacterMovement) Max%20Fly%20Speed))

(event Custom|Multicast_SetLookRotation%28Unreliable%29
  (params (LookRotation :type Rotator))
  (if (not (Pawn|IsLocallyControlled))
    (Variables|Default|SetLookRotation LookRotation)))

(event Custom|Server_SyncLookRotation%28Unreliable%29
  (params (LookRotation :type Rotator))
  (CallFunction|MulticastSetLookRotation(Unreliable) (Math|Rotator|MakeRotator (.roll LookRotation) (Math|Rotator|NormalizeAxis (.pitch LookRotation)) (Math|Rotator|NormalizeAxis (.yaw LookRotation)))))

(event Input|EnhancedActionEvents|EnhancedInputActionMoveVertical
  (params (ActionValue :type Float%20%28double-precision%29) (ElapsedSeconds :type Float%20%28double-precision%29) (TriggeredSeconds :type Float%20%28double-precision%29) (InputAction :type Input%20Action%20Object%20Reference :default "/Game/Misc/EnhancedInput/MoveVertical.MoveVertical"))
  (Pawn|Input|AddMovementInput (Math|Vector|VectorUp) ActionValue false))

(event Input|EnhancedActionEvents|EnhancedInputActionCameraRotate
  (params (ActionValue :type Vector%202D%20Structure) (ElapsedSeconds :type Float%20%28double-precision%29) (TriggeredSeconds :type Float%20%28double-precision%29) (InputAction :type Input%20Action%20Object%20Reference :default "/Game/Misc/EnhancedInput/CameraRotate.CameraRotate"))
  (bind (_x _y) (Math|Vector2D|BreakVector2D ActionValue))
  (bind _camerasens (Variables|Default|GetCameraSens))
  (Variables|Default|SetLookRotation (Math|Rotator|MakeRotator (.roll (Variables|Default|GetLookRotation)) (Math|Float|ClampAngle (+ (* _y _camerasens) (.pitch (Variables|Default|GetLookRotation))) -9e+01 9e+01) (+ (* _x _camerasens) (.yaw (Variables|Default|GetLookRotation))))))

(event Input|EnhancedActionEvents|EnhancedInputActionWheelBoth
  (params (ActionValue :type Float%20%28double-precision%29) (ElapsedSeconds :type Float%20%28double-precision%29) (TriggeredSeconds :type Float%20%28double-precision%29) (InputAction :type Input%20Action%20Object%20Reference :default "/Game/Misc/EnhancedInput/WheelBoth.WheelBoth"))
  (if (Variables|Default|GetZ_Pressed)
    (bind _output_get (Variables|Default|SetMoveSpeed (Math|Float|Clamp(Float) (+ (Variables|Default|GetMoveSpeed) (* (select (Variables|Default|GetShift) 1e+02 1e+01) ActionValue)) 0.0 1e+11)))
    (bind _output_get_2 (Variables|/Script/Engine.CharacterMovementComponent|SetMaxFlySpeed (Variables|Character|GetCharacterMovement) _output_get))
    (CallFunction|ServerChangeFlySpeed _output_get_2)
    (elif (Variables|Default|GetX_Pressed)
      (Variables|Default|SetCameraSens (+ (Variables|Default|GetCameraSens) (* (select (Variables|Default|GetShift) 0.1 0.01) ActionValue)))
      (elif (Variables|Default|GetC_Pressed)
        (Variables|/Script/Engine.SpringArmComponent|SetTargetArmLength (Variables|Default|GetSkySpringArm) (Math|Float|Clamp(Float) (+ (* ActionValue (select (Variables|Default|GetShift) -4e+02 -2e+01)) (Variables|/Script/Engine.SpringArmComponent|GetTargetArmLength (Variables|Default|GetSkySpringArm))) 0.0 1e+16))))))

(event Input|EnhancedActionEvents|EnhancedInputActionMove2D
  (params (ActionValue :type Vector%202D%20Structure) (ElapsedSeconds :type Float%20%28double-precision%29) (TriggeredSeconds :type Float%20%28double-precision%29) (InputAction :type Input%20Action%20Object%20Reference :default "/Game/Misc/EnhancedInput/Move2D.Move2D"))
  (bind (_x _y) (Math|Vector2D|BreakVector2D ActionValue))
  (bind _lookrotation (Variables|Default|GetLookRotation))
  (Pawn|Input|AddMovementInput (+ (* (Math|Vector|GetForwardVector _lookrotation) _y) (* (Math|Vector|GetRightVector _lookrotation) _x)) 1.0 false))

(event EventUnpossessed
  (params (OldController :type Controller%20Object%20Reference))
  (bind _w_cinematiccamera (Variables|Default|GetW_CinematicCamera))
  (Utilities|IsValid _w_cinematiccamera
    (:Is%20Valid
      (Widget|RemovefromParent _w_cinematiccamera))))

(event EventBeginPlay
  (bind _asbp_gis (Utilities|Casting|CastToBP_GIS (Game|GetGameInstance))
    (:then
      _)
    (:CastFailed
      _))
  (Variables|Default|SetBP_GIS _asbp_gis))

(event EventTick
  (params (DeltaSeconds :type Float%20%28single-precision%29))
  (Utilities|FlowControl|Sequence
    (:then_0
      (if (Pawn|IsLocallyControlled)
        (CallFunction|ServerSyncLookRotation(Unreliable) (Variables|Default|GetLookRotation))))
    (:then_1
      (Transformation|SetWorldRotation (Variables|Default|GetSkySpringArm) (Variables|Default|GetLookRotation) false false))))

(event EventPossessed
  (params (NewController :type Controller%20Object%20Reference))
  (bind _asbp_pcs (Utilities|Casting|CastToBP_PCS NewController))
  (bind _output_get (Variables|Default|SetBP_PCS _asbp_pcs))
  (Variables|Default|SetBP_PSS (Variables|/Game/Blueprints/BP_PCS.BP_PCS_C|GetBP_PSS _output_get))
  (Game|Player|SetViewTargetwithBlend (Variables|Default|GetBP_PCS) self 0.0 "VTBlend_Linear" 0.0 false)
  (Utilities|IsValid (Variables|Default|GetW_CinematicCamera)
    (:Is%20Valid
      (if (not (UserInterface|Viewport|IsinViewport (Variables|Default|GetW_CinematicCamera)))
        (UserInterface|Viewport|AddtoViewport (Variables|Default|GetW_CinematicCamera) 1 :!label _label)))
    (:Is%20Not%20Valid
      (bind _returnvalue (UserInterface|CreateWidget "/Game/Widgets/W_CinematicCamera.W_CinematicCamera_C" 0 self))
      (Variables|Default|SetW_CinematicCamera _returnvalue)
      (goto _label))))

(event Input|KeyboardEvents|E
  (params (Key :type Key%20Structure))
  (bind _returnvalue (Math|Random|RandomFloatinRange 0.05 0.2))
  (bind _returnvalue_2 (Math|Random|RandomFloatinRange 0.05 0.2))
  (bind _returnvalue_3 (Math|Random|RandomFloatinRange 0.05 0.2))
  (bind _camera (Variables|Default|GetCamera))
  (bind _returnvalue_4 (Transformation|GetWorldLocation _camera))
  (:Pressed
    (bind (_outhit _returnvalue_5) (Collision|LineTraceByChannel _returnvalue_4 (+ _returnvalue_4 (* (Math|Vector|GetForwardVector _camera) 5e+04)) "TraceTypeQuery1" false 0 "None"))
    (if _returnvalue_5
      (if (Class|AdianFL|ActorHasSkyTag (.HitActor (Collision|BreakHitResult _outhit)) "/Game/DataAssets/SkyTag/ST_PF_Normal.ST_PF_Normal")
        (if (not (== (Variables|Default|GetPF_Possess) (.HitActor (Collision|BreakHitResult _outhit))))
          (Actor|DestroyActor (.HitActor (Collision|BreakHitResult _outhit))))
        (else
          (bind _returnvalue_6 (Game|SpawnActorfromClass :Class "/Game/Blueprints/PF_Normal.PF_Normal_C" :SpawnTransform (Math|Transform|MakeTransform (+ (.ImpactPoint (Collision|BreakHitResult _outhit)) "0.000000,0.000000,150.000000") (Math|Rotator|MakeRotator 0.0 0.0 (.yaw (Transformation|GetWorldRotation (Variables|Default|GetCamera)))) "1.000000,1.000000,1.000000") :CollisionHandlingOverride "AlwaysSpawn" :TransformScaleMethod "MultiplyWithRoot" :Owner (Variables|/Game/Blueprints/BP_GIS.BP_GIS_C|GetBP_PCS (Variables|Default|GetBP_GIS)) :InitialEquipment (Utilities|Array|MakeArray "" (Utilities|Struct|MakeSlot "/Game/DataAssets/Item/I_EQOutfit_OldNosha.I_EQOutfit_OldNosha" 1 0) "" (Utilities|Struct|MakeSlot "/Game/DataAssets/Item/I_EQFeet_OldNosha.I_EQFeet_OldNosha" 1 0)) :CharacterBio (Utilities|Struct|MakeCharacterBio "None" true 0 (Utilities|Struct|MakeLinearColor _returnvalue_2 _returnvalue_3 _returnvalue 1.0) (Utilities|Struct|MakeLinearColor _returnvalue_2 _returnvalue_3 _returnvalue 1.0)) :PSS 0 :Instigator 0))
          (Rendering|SetActorHiddenInGame _returnvalue_6 false)
          (Utilities|Array|Add (Variables|Default|GetPF_Normals) (Utilities|Struct|MakeCinematicPF_Normals _returnvalue_6 "0.000000,0.000000,0.000000" "0.000000,0.000000,0.000000")))))))

(event Input|KeyboardEvents|R
  (params (Key :type Key%20Structure))
  (:Pressed
    (Utilities|IsValid (Variables|Default|GetCWS_Settings)
      (:Is%20Valid
        (if (UserInterface|Viewport|IsinViewport (Variables|Default|GetCWS_Settings))
          (Default|RemoveCWS (Variables|Default|GetBP_PSS) (Variables|Default|GetCWS_Settings) true)
          (else
            (Default|AddCWS (Variables|Default|GetBP_PSS) (Variables|Default|GetCWS_Settings) true true true "NewEnumerator2" :!label _label)
            (UserInterface|Viewport|AddtoViewport (Variables|Default|GetCWS_Settings) 15)
            (Default|SetMousetoCenter (Variables|Default|GetBP_PSS)))))
      (:Is%20Not%20Valid
        (bind _returnvalue (UserInterface|CreateWidget "/Game/Widgets/CWS/CWS_CinematicCameraSettings.CWS_CinematicCameraSettings_C" 0 self))
        (Variables|Default|SetCWS_Settings _returnvalue)
        (goto _label)))))

(event Input|KeyboardEvents|T
  (params (Key :type Key%20Structure))
  (bind _w_cinematiccamera (Variables|Default|GetW_CinematicCamera))
  (:Pressed
    (if (UserInterface|Viewport|IsinViewport _w_cinematiccamera)
      (Widget|RemovefromParent _w_cinematiccamera)
      (else
        (UserInterface|Viewport|AddtoViewport _w_cinematiccamera 1)))))

(event Input|KeyboardEvents|C
  (params (Key :type Key%20Structure))
  (:Pressed
    (Variables|Default|SetC_Pressed true))
  (:Released
    (Variables|Default|SetC_Pressed false)))

(event Input|KeyboardEvents|Z
  (params (Key :type Key%20Structure))
  (:Pressed
    (Variables|Default|SetZ_Pressed true))
  (:Released
    (Variables|Default|SetZ_Pressed false)))

(event Input|KeyboardEvents|LeftShift
  (params (Key :type Key%20Structure))
  (:Pressed
    (Variables|Default|SetShift true)
    (bind _output_get (Variables|/Script/Engine.CharacterMovementComponent|SetMaxFlySpeed (Variables|Character|GetCharacterMovement) (+ (Variables|Default|GetMoveSpeed) 3e+03)))
    (CallFunction|ServerChangeFlySpeed _output_get))
  (:Released
    (Variables|Default|SetShift false)
    (bind _output_get_2 (Variables|/Script/Engine.CharacterMovementComponent|SetMaxFlySpeed (Variables|Character|GetCharacterMovement) (Variables|Default|GetMoveSpeed)))
    (CallFunction|ServerChangeFlySpeed _output_get_2)))

(event Input|KeyboardEvents|X
  (params (Key :type Key%20Structure))
  (:Pressed
    (Variables|Default|SetX_Pressed true))
  (:Released
    (Variables|Default|SetX_Pressed false)))

(fn ConstructionScript)