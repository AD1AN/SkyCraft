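; Actor component that streams procedural sky-island chunks around its owner, ticking only on the server in the Sky Main level.
; When the owner changes chunk, it releases out-of-range chunks and claims those within a circular radius, reusing GM_Sky's shared registry through a per-chunk HMPR reference count.
; New chunks seed a random stream from coordinates and WorldSeed, occasionally spawning a VW_Island.
; Helpers release or transfer chunks and report island counts.
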(event Custom|Server_ReturnIslands
  (bind _islands (CallFunction|ReturnIslands))
  (CallFunction|ClientReturnIslands _islands))

(event Custom|Client_ReturnIslands
  (params (Islands :type Integer))
  (Default|CallIslandsReturn (Variables|Default|GetSGI) Islands))

(event EventTick
  (params (DeltaSeconds :type Float%20%28single-precision%29))
  (bind (_x _y) (CallFunction|GetActorChunkCors))
  (bind (_x_2 _y_2) (CallFunction|GetActorChunkCors))
  (if (not (and (== _x_2 (.x (Variables|Default|GetLastActorChunkCors))) (== _y_2 (.y (Variables|Default|GetLastActorChunkCors))))) ; Player has changed Chunk Coordinates
    (Variables|Default|SetLastActorChunkCors (Utilities|Struct|MakeIntVector _x _y 0))
    (CallFunction|DestroyChunks)
    (CallFunction|SpawnChunks)))

(event EventBeginPlay
  (Variables|Default|SetActor (Components|GetOwner))
  (bind _sgi (Class|BPISGI|GetSGI(Message) (Game|GetGameInstance)))
  (Variables|Default|SetSGI _sgi)
  (if (Networking|IsServer)
    (switch Utilities|FlowControl|Switch|SwitchonCurrentLevel (Variables|/Game/Blueprints/SGI.SGI_C|GetCurrentLevel (Variables|Default|GetSGI))
      (:NewEnumerator1
        (if (Class|LowEntryExtendedStandardLibrary|ShippingBuild)
          _
          (else
            (Variables|Default|SetShippingRenderRangeXY (Variables|Default|GetTestRenderRangeXY))))
        (bind _asgm_sky (Utilities|Casting|CastToGM_Sky (Game|GetGameMode)))
        (Variables|Default|SetGM_Sky _asgm_sky)
        (Components|Tick|SetComponentTickEnabled true)))))

(fn GetActorChunkCors
  (bind _actor (Variables|Default|GetActor))
  (bind _chunksizexy (Variables|Default|GetChunkSizeXY))
  (bind _returnvalue (Transformation|GetActorLocation _actor))
  (bind _returnvalue_2 (/ _returnvalue _chunksizexy))
  (bind (_x _y) (Math|Vector|BreakVector _returnvalue_2))
  (return (Math|Float|Round _x) (Math|Float|Round _y)))

(fn DestroyChunks
  (bind (_x _y) (CallFunction|GetActorChunkCors))
  (bind _chunksizexy (Variables|Default|GetChunkSizeXY))
  (bind _chunksizexy_2 (Variables|Default|GetChunkSizeXY))
  (for (_array_element _array_index) (Variables|Default|GetHMPR_SpawnedChunksCors)
    (LocalVariables|SetTempIndex _array_index)
    (if (>= (Math|Vector|Distance(Vector) (Math|Vector|MakeVector (* (.X (Utilities|Struct|BreakIntVector _array_element)) _chunksizexy) (* (.Y (Utilities|Struct|BreakIntVector _array_element)) _chunksizexy) 0.0) (Math|Vector|MakeVector (* _x _chunksizexy_2) (* _y _chunksizexy_2) 0.0)) (* (Variables|Default|GetShippingRenderRangeXY) (Variables|Default|GetChunkSizeXY)))
      (Utilities|Array|Add (LocalVariables|GetIndexForRemoval) (LocalVariables|GetTempIndex))))
  (for (_array_element_2 _array_index_2) (LocalVariables|GetIndexForRemoval)
    (Variables|/Game/Blueprints/SkyMain/SA_Chunk_Islands.SA_Chunk_Islands_C|SetHMPR (Utilities|Array|Get(acopy) (Variables|Default|GetHMPR_SpawnedChunks) (- _array_element_2 _array_index_2)) (- (Variables|/Game/Blueprints/SkyMain/SA_Chunk_Islands.SA_Chunk_Islands_C|GetHMPR (Utilities|Array|Get(acopy) (Variables|Default|GetHMPR_SpawnedChunks) (- _array_element_2 _array_index_2))) 1))
    (Utilities|Array|RemoveIndex (Variables|Default|GetHMPR_SpawnedChunksCors) (- _array_element_2 _array_index_2))
    (Utilities|Array|RemoveIndex (Variables|Default|GetHMPR_SpawnedChunks) (- _array_element_2 _array_index_2))))

(fn SpawnChunks
  (bind (_x _y) (CallFunction|GetActorChunkCors))
  (bind _shippingrenderrangexy (Variables|Default|GetShippingRenderRangeXY))
  (bind _chunksizexy (Variables|Default|GetChunkSizeXY))
  (bind _chunksizexy_2 (Variables|Default|GetChunkSizeXY))
  (bind _gm_sky (Variables|Default|GetGM_Sky))
  (bind _shippingrenderrangexy_2 (Variables|Default|GetShippingRenderRangeXY))
  (bind _gm_sky_2 (Variables|Default|GetGM_Sky))
  (for _index (range (* _shippingrenderrangexy_2 -1) _shippingrenderrangexy_2)
    (LocalVariables|SetTempX _index)
    (for _index_2 (range (* _shippingrenderrangexy -1) _shippingrenderrangexy)
      (LocalVariables|SetTempY _index_2)
      (LocalVariables|SetChunkCors (Utilities|Struct|MakeIntVector (+ _x (LocalVariables|GetTempX)) (+ _y (LocalVariables|GetTempY))))
      (if (and (not (Utilities|Array|ContainsItem (Variables|Default|GetHMPR_SpawnedChunksCors) (LocalVariables|GetChunkCors))) (< (Math|Vector|VectorLength (Math|Vector|MakeVector (* (LocalVariables|GetTempX) _chunksizexy) (* (LocalVariables|GetTempY) _chunksizexy) 0.0)) (* (Variables|Default|GetShippingRenderRangeXY) (Variables|Default|GetChunkSizeXY))))
        (if (Utilities|Array|ContainsItem (Variables|/Game/Blueprints/SkyMain/GM_Sky.GM_Sky_C|GetSpawnedChunkIslandsCors (Variables|Default|GetGM_Sky)) (LocalVariables|GetChunkCors))
          (Utilities|Array|Add (Variables|Default|GetHMPR_SpawnedChunksCors) (LocalVariables|GetChunkCors))
          (Utilities|Array|Add (Variables|Default|GetHMPR_SpawnedChunks) (Utilities|Array|Get(acopy) (Variables|/Game/Blueprints/SkyMain/GM_Sky.GM_Sky_C|GetSpawnedChunkIslands _gm_sky_2) (Utilities|Array|FindItem (Variables|/Game/Blueprints/SkyMain/GM_Sky.GM_Sky_C|GetSpawnedChunkIslandsCors _gm_sky_2) (LocalVariables|GetChunkCors))))
          (Variables|/Game/Blueprints/SkyMain/SA_Chunk_Islands.SA_Chunk_Islands_C|SetHMPR (Utilities|Array|Get(acopy) (Variables|/Game/Blueprints/SkyMain/GM_Sky.GM_Sky_C|GetSpawnedChunkIslands _gm_sky_2) (Utilities|Array|FindItem (Variables|/Game/Blueprints/SkyMain/GM_Sky.GM_Sky_C|GetSpawnedChunkIslandsCors _gm_sky_2) (LocalVariables|GetChunkCors))) (+ (Variables|/Game/Blueprints/SkyMain/SA_Chunk_Islands.SA_Chunk_Islands_C|GetHMPR (Utilities|Array|Get(acopy) (Variables|/Game/Blueprints/SkyMain/GM_Sky.GM_Sky_C|GetSpawnedChunkIslands _gm_sky_2) (Utilities|Array|FindItem (Variables|/Game/Blueprints/SkyMain/GM_Sky.GM_Sky_C|GetSpawnedChunkIslandsCors _gm_sky_2) (LocalVariables|GetChunkCors)))) 1))
          (else
            ;[1 1 1] SpawnChunk
            (bind _returnvalue (Game|SpawnActorfromClass "/Game/Blueprints/SkyMain/SA_Chunk_Islands.SA_Chunk_Islands_C" (Math|Transform|MakeTransform (Math|Vector|MakeVector (* (.x (LocalVariables|GetChunkCors)) _chunksizexy_2) (* (.y (LocalVariables|GetChunkCors)) _chunksizexy_2) 5e+03) "0, 0, 0" "1.000000,1.000000,1.000000") "AlwaysSpawn" 0 (Variables|Default|GetGM_Sky) 1 0))
            (LocalVariables|SetSpawnedChunk _returnvalue)
            (Utilities|FlowControl|Sequence
              (:then_0
                (Utilities|Array|Add (Variables|/Game/Blueprints/SkyMain/GM_Sky.GM_Sky_C|GetSpawnedChunkIslands _gm_sky) (LocalVariables|GetSpawnedChunk))
                (Utilities|Array|Add (Variables|/Game/Blueprints/SkyMain/GM_Sky.GM_Sky_C|GetSpawnedChunkIslandsCors _gm_sky) (LocalVariables|GetChunkCors))
                (Utilities|Array|Add (Variables|Default|GetHMPR_SpawnedChunks) (LocalVariables|GetSpawnedChunk))
                (Utilities|Array|Add (Variables|Default|GetHMPR_SpawnedChunksCors) (LocalVariables|GetChunkCors)))
              (:then_1
                (LocalVariables|SetSpawnedChunkCors (Class|KismetMathLibrary|FTruncVector (Transformation|GetActorLocation (LocalVariables|GetSpawnedChunk))))
                (bind _output_get (LocalVariables|SetSpawnedChunkStream (Math|Random|MakeRandomStream (+ (CallFunction|Int->Stream->Int (.x (LocalVariables|GetSpawnedChunkCors))) (CallFunction|Int->Stream->Int (CallFunction|Int->Stream->Int (.y (LocalVariables|GetSpawnedChunkCors)))) (Variables|/Game/Blueprints/SkyMain/GM_Sky.GM_Sky_C|GetWorldSeed (Variables|Default|GetGM_Sky))))))
                (if (Class|KismetMathLibrary|RandomBoolwithWeightfromStream 0.05 _output_get)
                  (Variables|/Game/Blueprints/SkyMain/SA_Chunk_Islands.SA_Chunk_Islands_C|SetChunkSeed (LocalVariables|GetSpawnedChunk) (Class|KismetMathLibrary|RandomIntegerfromStream 2147483647 (LocalVariables|GetSpawnedChunkStream)))
                  (Variables|/Game/Blueprints/SkyMain/SA_Chunk_Islands.SA_Chunk_Islands_C|SetChunkScale (LocalVariables|GetSpawnedChunk) (Math|Random|RandomIntegerinRangefromStream 50 200 (LocalVariables|GetSpawnedChunkStream)))
                  (bind _returnvalue_2 (Game|SpawnActorfromClass "/Game/Blueprints/SkyMain/VW_Island.VW_Island_C" (Math|Transform|MakeTransform (Math|Vector|MakeVector (Math|Random|RandomFloatinRangefromStream (+ (* (.x (Components|Box|GetScaledBoxExtent (Variables|/Game/Blueprints/SkyMain/SA_Chunk_Islands.SA_Chunk_Islands_C|GetIslandBox (LocalVariables|GetSpawnedChunk)))) -1.0) (.x (Transformation|GetWorldLocation (Variables|/Game/Blueprints/SkyMain/SA_Chunk_Islands.SA_Chunk_Islands_C|GetIslandBox (LocalVariables|GetSpawnedChunk))))) (+ (.x (Components|Box|GetScaledBoxExtent (Variables|/Game/Blueprints/SkyMain/SA_Chunk_Islands.SA_Chunk_Islands_C|GetIslandBox (LocalVariables|GetSpawnedChunk)))) (.x (Transformation|GetWorldLocation (Variables|/Game/Blueprints/SkyMain/SA_Chunk_Islands.SA_Chunk_Islands_C|GetIslandBox (LocalVariables|GetSpawnedChunk))))) (LocalVariables|GetSpawnedChunkStream)) (Math|Random|RandomFloatinRangefromStream (+ (* (.y (Components|Box|GetScaledBoxExtent (Variables|/Game/Blueprints/SkyMain/SA_Chunk_Islands.SA_Chunk_Islands_C|GetIslandBox (LocalVariables|GetSpawnedChunk)))) -1.0) (.y (Transformation|GetWorldLocation (Variables|/Game/Blueprints/SkyMain/SA_Chunk_Islands.SA_Chunk_Islands_C|GetIslandBox (LocalVariables|GetSpawnedChunk))))) (+ (.y (Components|Box|GetScaledBoxExtent (Variables|/Game/Blueprints/SkyMain/SA_Chunk_Islands.SA_Chunk_Islands_C|GetIslandBox (LocalVariables|GetSpawnedChunk)))) (.y (Transformation|GetWorldLocation (Variables|/Game/Blueprints/SkyMain/SA_Chunk_Islands.SA_Chunk_Islands_C|GetIslandBox (LocalVariables|GetSpawnedChunk))))) (LocalVariables|GetSpawnedChunkStream)) (Math|Random|RandomFloatinRangefromStream 7e+03 1.5e+04 (LocalVariables|GetSpawnedChunkStream))) "0, 0, 0" "1.000000,1.000000,1.000000") "Undefined" 0 0))
                  (bind _output_get_2 (Variables|/Game/Blueprints/SkyMain/SA_Chunk_Islands.SA_Chunk_Islands_C|SetIsland (LocalVariables|GetSpawnedChunk) _returnvalue_2))
                  (Variables|/Game/Blueprints/SkyMain/VW_Island.VW_Island_C|SetChunk _output_get_2 (LocalVariables|GetSpawnedChunk)))))))))))

(fn ReturnIslands
  (for _array_element (Variables|Default|GetHMPR_SpawnedChunks)
    (Utilities|IsValid (Variables|/Game/Blueprints/SkyMain/SA_Chunk_Islands.SA_Chunk_Islands_C|GetIsland _array_element)
      (:Is%20Valid
        (LocalVariables|Set_Islands (+ 1 (LocalVariables|Get_Islands))))))
  (return (LocalVariables|Get_Islands)))

(fn MinusSpawnedChunks
  (for _array_element (Variables|Default|GetHMPR_SpawnedChunks)
    (Variables|/Game/Blueprints/SkyMain/SA_Chunk_Islands.SA_Chunk_Islands_C|SetHMPR _array_element (- (Variables|/Game/Blueprints/SkyMain/SA_Chunk_Islands.SA_Chunk_Islands_C|GetHMPR _array_element) 1)))
  (Utilities|Array|Clear (Variables|Default|GetHMPR_SpawnedChunks))
  (Utilities|Array|Clear (Variables|Default|GetHMPR_SpawnedChunksCors)))

(fn TransferChunks
  (params (FromGenerator :type Generator%20Islands%20Object%20Reference))
  (Variables|Default|SetHMPR_SpawnedChunks (Variables|Generator_Islands_C|GetHMPR_SpawnedChunks FromGenerator))
  (Variables|Default|SetHMPR_SpawnedChunksCors (Variables|Generator_Islands_C|GetHMPR_SpawnedChunksCors FromGenerator))
  (Variables|Default|SetLastActorChunkCors (Variables|Generator_Islands_C|GetLastActorChunkCors FromGenerator))
  (return))