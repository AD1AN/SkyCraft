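; BP_GSS holds a saved-player map along with references to the game instance and the sky actor.
; BeginPlay caches the BP_GIS game instance, then finds and stores the level's Ultra_Dynamic_Sky actor, skipping that lookup if the cast fails.
; Multicast_SetSavedPlayers pairs parallel key and value arrays by index and adds them to SavedPlayers.
; Despite the Multicast name, the map is written only on the authority side.
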(event Custom|Multicast_SetSavedPlayers
  (params (Keys :type Array%20of%20Strings) (Values :type Array%20of%20SS%20Player%20Structures))
  (Networking|SwitchHasAuthority
    (:Authority
      (for (_array_element _array_index) Keys
        (Utilities|Map|Add (Variables|Default|GetSavedPlayers) _array_element (Utilities|Array|Get(acopy) Values _array_index))))))

(event EventBeginPlay
  (bind _asbp_gis (Utilities|Casting|CastToBP_GIS (Game|GetGameInstance)))
  (Variables|Default|SetBP_GIS _asbp_gis)
  (bind _returnvalue (Actor|GetActorOfClass "/Game/UltraDynamicSky/Blueprints/Ultra_Dynamic_Sky.Ultra_Dynamic_Sky_C"))
  (Variables|Default|SetUDS _returnvalue))

(fn ConstructionScript)