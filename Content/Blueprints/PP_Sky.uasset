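; PP_Sky is a per-player hub owned by the Sky player controller, linking it to the player's Island, Normal, Spirit and Dead forms.
; Init caches the controller, game instance and server game mode, and possession multicasts store each form reference.
; It routes chat between the Normal form's widget and GM_Sky, and relays interaction interrupts to server and client handlers.
; Server events handle island pawn control, Essence transfer and stopping IA on IslandArchon.
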(event Custom|Server_StopIA
  (Default|StopIA (Variables|Default|GetIslandArchon)))

(event Custom|Multicast_SetIslandArchon
  (params (IslandArchon :type Island%20Archon%20Object%20Reference))
  (bind _pc_sky (Variables|Default|GetPC_Sky))
  (bind _output_get (Variables|Default|SetIslandArchon IslandArchon))
  (Utilities|IsValid _pc_sky
    (:Is%20Valid
      (Variables|/Game/Blueprints/PC_Sky.PC_Sky_C|SetIslandArchon _pc_sky _output_get))))

(event Custom|Server_Interrupt
  (params (InterruptActor :type Object%20Object%20Reference) (InterruptedBy :type E_InterruptedBy%20Enum :default "NewEnumerator0") (InteractKey :type E_InteractKey%20Enum :default "NewEnumerator0") (InteractedPawn :type Pawn%20Object%20Reference) (InteractedPC_Sky :type PC%20Sky%20Object%20Reference) (InteractedPP_Sky :type PP%20Sky%20Object%20Reference))
  (bind _interactsystem (Class|BPIInteractSystem|GetInteractSystem(Message) InterruptActor))
  (Default|RemoveProlonged _interactsystem InteractedPawn)
  (Default|CallServerInterrupted _interactsystem InterruptedBy InteractKey InteractedPawn)
  (Class|BPIInteractSystem|ServerInterrupt(Message) InterruptActor InterruptedBy InteractKey InteractedPawn InteractedPC_Sky InteractedPP_Sky)
  (CallFunction|ClientInterrupt(Don'tCallThis!) InterruptActor InterruptedBy InteractKey InteractedPawn InteractedPC_Sky InteractedPP_Sky))

(event Custom|Multicast_Init
  (if (not (Variables|Default|GetInitialized))
    (Variables|Default|SetInitialized true)
    (bind _assgi (Utilities|Casting|CastToSGI (Game|GetGameInstance))
      (:then
        _)
      (:CastFailed
        _))
    (Variables|Default|SetSGI _assgi)
    (bind _pc_sky (Class|BPIPGSky|GetPCSky(Message) (Components|GetOwner)))
    (Variables|Default|SetPC_Sky _pc_sky)
    (Utilities|IsOwner
      (:Server
        (bind _asgm_sky (Utilities|Casting|CastToGM_Sky (Game|GetGameMode)))
        (Variables|Default|SetGM_Sky _asgm_sky))
      (:OwningClient
        (Variables|/Game/Blueprints/SGI.SGI_C|SetPP_Sky (Variables|Default|GetSGI) self)))))

(event Custom|EnsureInit
  (if (not (Variables|Default|GetInitialized))
    (Variables|Default|SetInitialized true)
    (bind _assgi (Utilities|Casting|CastToSGI (Game|GetGameInstance))
      (:then
        _)
      (:CastFailed
        _))
    (Variables|Default|SetSGI _assgi)
    (bind _pc_sky (Class|BPIPGSky|GetPCSky(Message) (Components|GetOwner)))
    (Variables|Default|SetPC_Sky _pc_sky)
    (Utilities|IsOwner
      (:Server
        (bind _asgm_sky (Utilities|Casting|CastToGM_Sky (Game|GetGameMode)))
        (Variables|Default|SetGM_Sky _asgm_sky))
      (:OwningClient
        (Variables|/Game/Blueprints/SGI.SGI_C|SetPP_Sky (Variables|Default|GetSGI) self)))))

(event Custom|Server_IA_GiveEssence
  (params (GiveEssence :type S%20Essence%20Structure))
  (Variables|/Game/Blueprints/IslandArchon.IslandArchon_C|SetEssence (Variables|Default|GetIslandArchon) (CallFunction|AddEssence GiveEssence (Variables|/Game/Blueprints/IslandArchon.IslandArchon_C|GetEssence (Variables|Default|GetIslandArchon))))
  (Variables|/Game/Blueprints/PF_Normal.PF_Normal_C|SetEssence (Variables|PlayerForms|GetPF_Normal) (CallFunction|SubtractEssence (Variables|/Game/Blueprints/PF_Normal.PF_Normal_C|GetEssence (Variables|PlayerForms|GetPF_Normal)) GiveEssence)))

(event Custom|Server_SendMessage
  (params (Sender :type String) (Message :type String))
  ;[1 1 1] Chat
  (Default|SendMessagetoEveryone (Variables|Default|GetGM_Sky) Sender Message))

(event Custom|Client_Interrupt%20%28Don't%20call%20this!%29
  (params (InterruptActor :type Object%20Object%20Reference) (InterruptedBy :type E_InterruptedBy%20Enum :default "NewEnumerator0") (InteractKey :type E_InteractKey%20Enum :default "NewEnumerator0") (InteractedPawn :type Pawn%20Object%20Reference) (InteractedPC_Sky :type PC%20Sky%20Object%20Reference) (InteractedPP_Sky :type PP%20Sky%20Object%20Reference))
  (bind _interactsystem (Class|BPIInteractSystem|GetInteractSystem(Message) InterruptActor))
  (Default|CallClientInterrupted _interactsystem InterruptedBy InteractKey InteractedPawn)
  (Class|BPIInteractSystem|ClientInterrupt(Message) InterruptActor InterruptedBy InteractKey InteractedPawn InteractedPC_Sky InteractedPP_Sky))

(event Custom|AddMessageToChat
  (params (Sender :type String) (Message :type String))
  ;[1 1 1] Chat
  (Default|AddMessagetoChat (Variables|/Game/Blueprints/PF_Normal.PF_Normal_C|GetW_PF_Normal (Variables|PlayerForms|GetPF_Normal)) Sender Message))

(event Custom|Multicast_PlayerForm_Possessed
  (params (CurrentPlayerForm :type E_PlayerForm%20Enum :default "NewEnumerator0") (PlayerForm_Possess :type Actor%20Object%20Reference))
  (bind _output_get (Variables|PlayerForms|SetCurrentPF CurrentPlayerForm))
  (bind (_pc_sky _pf_island _pf_normal _pf_spirit _pf_dead) (Class|BPIPlayerForm|GetPlayerForm(Message) PlayerForm_Possess))
  (switch Utilities|FlowControl|Switch|SwitchonE_PlayerForm _output_get
    (:NewEnumerator0
      (Variables|PlayerForms|SetPF_Island _pf_island))
    (:NewEnumerator2
      (Variables|PlayerForms|SetPF_Normal _pf_normal))
    (:NewEnumerator3
      (Variables|PlayerForms|SetPF_Spirit _pf_spirit))
    (:NewEnumerator1
      (Variables|PlayerForms|SetPF_Dead _pf_dead))))

(event Custom|Multicast_StoredQSI
  (params (StoredQSI :type Integer))
  (Variables|Default|SetStoredQSI StoredQSI))

(event Custom|TypingChat
  (bind _pf_normal (Variables|PlayerForms|GetPF_Normal))
  (bind _w_pf_normal (Variables|/Game/Blueprints/PF_Normal.PF_Normal_C|GetW_PF_Normal _pf_normal))
  ;[1 1 1] Chat
  (Input|SetInputModeGameandUI (Variables|Default|GetPC_Sky) (Variables|/Game/Widgets/W_PF_Normal.W_PF_Normal_C|GetMessageInput (Variables|/Game/Blueprints/PF_Normal.PF_Normal_C|GetW_PF_Normal (Variables|PlayerForms|GetPF_Normal))) "DoNotLock" true)
  (Variables|/Script/Engine.PlayerController|SetbShowMouseCursor (Variables|Default|GetPC_Sky) true)
  (Class|UserWidget|StopAnimation _w_pf_normal (Variables|/Game/Widgets/W_PF_Normal.W_PF_Normal_C|GetHideChat _w_pf_normal))
  (Widget|SetRenderOpacity (Variables|/Game/Widgets/W_PF_Normal.W_PF_Normal_C|GetChat _w_pf_normal) 1.0))

(event Custom|Server_SetPawnIslandControl
  (params (Pawn :type Pawn%20Object%20Reference))
  (bind _islandarchon (Variables|Default|GetIslandArchon))
  (bind _pawn_island_control (Variables|/Game/Blueprints/IslandArchon.IslandArchon_C|GetPawn%20Island%20Control _islandarchon))
  (Default|MulticastPossessControlPawn _pawn_island_control Pawn self)
  (Game|Player|SetViewTargetwithBlend (Variables|Default|GetPC_Sky) _pawn_island_control 1.0 "VTBlend_EaseInOut" 2.0 false)
  (Default|PossessPawn (Variables|Default|GetPC_Sky) _pawn_island_control true))

(event EventBeginPlay
  (CallFunction|EnsureInit)
  (Utilities|IsOwner
    (:OwningClient
      (Default|ClientStartPlayer (Variables|Default|GetPC_Sky)))))

(event Input|ActionEvents|InputActionChat
  (params (Key :type Key%20Structure :default "None"))
  ;[1 1 1] Chat
  (:Pressed
    (CallFunction|TypingChat)))

(fn ConstructionScript)

(fn GetPlayerForm
  (return (Variables|Default|GetPC_Sky) (Variables|PlayerForms|GetPF_Island) (Variables|PlayerForms|GetPF_Normal) (Variables|PlayerForms|GetPF_Spirit) (Variables|PlayerForms|GetPF_Dead)))