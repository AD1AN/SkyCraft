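; AN_PlayAttachedSound is an animation notify that plays a configurable sound attached to the animated mesh component.
; When triggered, it spawns the sound with the chosen attenuation settings, using either fixed volume and pitch or a random value within a range for each, controlled by separate toggles.
; It displays as "Sound" on the animation timeline.
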(fn ReceivedNotify
  (params (MeshComp :type Skeletal%20Mesh%20Component%20Object%20Reference) (Animation :type Anim%20Sequence%20Base%20Object%20Reference) (EventReference :type Anim%20Notify%20Event%20Reference%20Structure%20%28by%20ref%29))
  (Audio|SpawnSoundAttached (Variables|AnimNotify|GetSound) MeshComp "None" "0, 0, 0" "0, 0, 0" "KeepRelativeOffset" false (select (Variables|AnimNotify|GetVolumeRandom) (Math|Random|RandomFloatinRange (Variables|AnimNotify|GetVolume) (Variables|AnimNotify|GetVolumeMax)) (Variables|AnimNotify|GetVolume)) (select (Variables|AnimNotify|GetPitchRandom) (Math|Random|RandomFloatinRange (Variables|AnimNotify|GetPitch) (Variables|AnimNotify|GetPitchMax)) (Variables|AnimNotify|GetPitch)) 0.0 (Variables|AnimNotify|GetAttenuationSettings) 0)
  (return true))

(fn GetNotifyName
  (return "Sound"))