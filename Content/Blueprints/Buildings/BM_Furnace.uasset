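; Placeable furnace building that burns fuel to turn input items into outputs using fuel and recipe data tables.
; Server-bound inventory events consume items and enable Tick, which counts down fuel and advances cooking, then disables itself without fuel or work.
; RepNotifies update fuel timing, listeners and the fire light, while interaction opens a client widget.
; It also saves and restores its state, checks placement space and drops items when destroyed or dismantled.
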(event OnDie(HealthSystem)
  (Networking|SwitchHasAuthority
    (:Authority
      (CallFunction|DropItems))))

(event Custom|SAE_Inventory_Input
  (params (SlotIndex :type Integer))
  (Utilities|IsValid (.da_item (Variables|Default|GetCurrentFuel)) ; Has CurrentFuel
    (:Is%20Valid
      (Utilities|IsValid (.da_item (.output (Variables|Default|GetCurrentOutput))) ; Has CurrentOutput
        (:Is%20Valid
          (Actor|Tick|SetActorTickEnabled true))
        (:Is%20Not%20Valid
          (Utilities|IsValid (.da_item (Utilities|Array|Get(acopy) (Variables|/Script/SkyCraft.Inventory|GetSlots (Variables|Default|GetInventoryOutput)))) ; OutputSlot
            (:Is%20Valid
              (bind (_valid _s_furnaceoutput) (CallFunction|IsInputValid))
              (if _valid
                (if (== (.da_item (.Output (Utilities|Struct|BreakS_FurnaceOutput _s_furnaceoutput))) (.da_item (Utilities|Array|Get(acopy) (Variables|/Script/SkyCraft.Inventory|GetSlots (Variables|Default|GetInventoryOutput)))))
                  (CallFunction|ConsumeInput _s_furnaceoutput)
                  (Actor|Tick|SetActorTickEnabled true)
                  (else
                    (CallFunction|SetNoSpace true)))))
            (:Is%20Not%20Valid
              (CallFunction|SetNoSpace false)
              (bind (_valid_2 _s_furnaceoutput_2) (CallFunction|IsInputValid))
              (if _valid_2
                (CallFunction|ConsumeInput _s_furnaceoutput_2)
                (Actor|Tick|SetActorTickEnabled true)))))))
    (:Is%20Not%20Valid
      (CallFunction|OnFuel))))

(event Custom|OnChangeSlot_Event
  (params (SlotIndex :type Integer))
  (CallFunction|OnFuel))

(event EventBeginPlay
  (Networking|SwitchHasAuthority
    (:Authority
      (EventDispatchers|BindEventtoOnChangeSlot (Variables|Default|GetInventoryFuel) (delegate Custom|OnChangeSlot_Event))
      (EventDispatchers|BindEventtoOnChangeSlot (Variables|Default|GetInventoryInput) (delegate Custom|SAE_Inventory_Input))
      (EventDispatchers|BindEventtoOnChangeSlot (Variables|Default|GetInventoryOutput) (delegate Custom|SAE_Inventory_Input)))))

(event EventTick
  (params (DeltaSeconds :type Float%20%28single-precision%29))
  (if (> (Variables|Default|GetCurrentFuelTime) 0.0) ; Have Fuel
    (Variables|Default|SetCurrentFuelTime (- (Variables|Default|GetCurrentFuelTime) 1.0)) ; Burn fuel
    (Utilities|FlowControl|Sequence
      (:then_0
        (Utilities|IsValid (.da_item (.output (Variables|Default|GetCurrentOutput)))
          (:Is%20Valid
            (Variables|Default|SetCurrentCookTime (+ (Variables|Default|GetCurrentCookTime) 1.0)) ; Cooking
            (if (>= (Variables|Default|GetCurrentCookTime) (Variables|Default|GetMaxCookTime)) ; COOKED?
              (Variables|Default|SetCurrentCookTime 0.0)
              (Utilities|FlowControl|Sequence
                (:then_0
                  (Utilities|IsValid (.da_item (.Output (Utilities|Struct|BreakS_FurnaceOutput (Variables|Default|GetCurrentOutput))))
                    (:Is%20Valid
                      (if (Variables|/Script/SkyCraft.DA_Item|GetbCanStack (.da_item (.Output (Utilities|Struct|BreakS_FurnaceOutput (Variables|Default|GetCurrentOutput)))))
                        (Class|Inventory|InsertSlot (Variables|Default|GetInventoryOutput) (.output (Variables|Default|GetCurrentOutput)))
                        (else
                          (CallFunction|SetNoSpace true))))
                    (:Is%20Not%20Valid
                      (CallFunction|AdianPrintError "ERROR: IDK WTF I JUST COOKED"))))
                (:then_1
                  (Variables|Default|SetCurrentOutput "") ; empty
                  (bind (_valid _s_furnaceoutput) (CallFunction|IsInputValid))
                  (if _valid
                    (CallFunction|ConsumeInput _s_furnaceoutput))))))))
      (:then_1
        (if (<= (Variables|Default|GetCurrentFuelTime) 0.0) ; Fuel is out
          (Variables|Default|SetCurrentFuelTime 0.0)
          (Variables|Default|SetCurrentFuel "") ; empty
          (bind (_has _index _s_fuel) (CallFunction|HasFuel))
          (if _has
            (Utilities|IsValid (.da_item (.output (Variables|Default|GetCurrentOutput)))
              (:Is%20Valid
                (CallFunction|ConsumeFuel _index _s_fuel))
              (:Is%20Not%20Valid
                (Actor|Tick|SetActorTickEnabled false :!label _label)))
            (else
              (goto _label))))))
    (else
      (Actor|Tick|SetActorTickEnabled false))))

(event EventDismantled
  (Networking|SwitchHasAuthority
    (:Authority
      (CallFunction|DropItems))))

(fn ConstructionScript
  (|CallParentFunction))

(fn SaveBuildingParameters
  (bind _rootcomponent (Variables|Transformation|GetRootComponent))
  (return (Utilities|Struct|MakeBuildingParameters (Utilities|Array|MakeArray (Variables|/Script/Engine.SceneComponent|GetRelativeLocation _rootcomponent)) (Utilities|Array|MakeArray (Variables|/Script/Engine.SceneComponent|GetRelativeRotation _rootcomponent)) (Utilities|Array|MakeArray (Utilities|Struct|MakeArrayInventorySlots (Variables|/Script/SkyCraft.Inventory|GetSlots (Variables|Default|GetInventoryInput))) (Utilities|Struct|MakeArrayInventorySlots (Variables|/Script/SkyCraft.Inventory|GetSlots (Variables|Default|GetInventoryOutput))) (Utilities|Struct|MakeArrayInventorySlots (Variables|/Script/SkyCraft.Inventory|GetSlots (Variables|Default|GetInventoryFuel))) (Utilities|Struct|MakeArrayInventorySlots (Utilities|Array|MakeArray (.input (Variables|Default|GetCurrentOutput)))) (Utilities|Struct|MakeArrayInventorySlots (Utilities|Array|MakeArray (Utilities|Struct|MakeSlot (.da_item (Variables|Default|GetCurrentFuel)) 1 0)))) 0 (Utilities|Array|MakeArray (Variables|Default|GetCurrentFuelTime) (Variables|Default|GetCurrentCookTime)) 0 0 0 (Utilities|Array|MakeArray (Class|Actor|IsActorTickEnabled)))))

(fn LoadBuildingParameters
  (params (BuildingParameters :type Building%20Parameters%20Structure))
  (bind (_vectors _rotations _arrayinventoryslots _datetimes _floats _integers _arrayids _bytes _booleans) (Utilities|Struct|BreakBuildingParameters BuildingParameters))
  (bind _output (Utilities|Array|Get(acopy) _arrayinventoryslots 4))
  (bind _output_2 (Utilities|Array|Get(acopy) _arrayinventoryslots 3))
  (bind _output_3 (Utilities|Array|Get(acopy) (.inventoryslots _output)))
  (bind _output_4 (Utilities|Array|Get(acopy) (.inventoryslots _output_2)))
  (Transformation|SetRelativeLocationAndRotation (Variables|Transformation|GetRootComponent) (Utilities|Array|Get(acopy) _vectors) (Utilities|Array|Get(acopy) _rotations) false true)
  (for _index (range 0 2)
    (Variables|/Script/SkyCraft.Inventory|SetSlots (Utilities|Select :Index _index :Option%200 (Variables|Default|GetInventoryInput) :Option%201 (Variables|Default|GetInventoryOutput) :Option%202 (Variables|Default|GetInventoryFuel)) (.inventoryslots (Utilities|Array|Get(acopy) _arrayinventoryslots _index))))
  (Utilities|FlowControl|Sequence
    (:then_0
      (Utilities|IsValid (.da_item _output_4)
        (:Is%20Valid
          (bind _outrownames (DataTable|GetDataTableRowNames "/Game/Blueprints/BuildingSystem/Furnace/DT_FurnaceOutput.DT_FurnaceOutput"))
          (bind _array_element (Utilities|Array|ForEachLoopwithBreak _outrownames :!label _label)
            (:LoopBody
              (bind _returnvalue (Utilities|GetDataTableRow "/Game/Blueprints/BuildingSystem/Furnace/DT_FurnaceOutput.DT_FurnaceOutput" _array_element)
                (:then
                  (if (== (.da_item (Utilities|Struct|BreakS_FurnaceOutput _returnvalue)) (.da_item _output_4))
                    (bind _output_get (Variables|Default|SetCurrentOutput _returnvalue))
                    (Variables|Default|SetMaxCookTime (.cooktime _output_get))
                    (goto _label Break)))))))))
    (:then_1
      (Utilities|IsValid (.da_item _output_3)
        (:Is%20Valid
          (bind _outrownames_2 (DataTable|GetDataTableRowNames "/Game/Blueprints/BuildingSystem/Furnace/DT_FurnaceFuel.DT_FurnaceFuel"))
          (for _array_element_2 _outrownames_2
            (bind _returnvalue_2 (Utilities|GetDataTableRow "/Game/Blueprints/BuildingSystem/Furnace/DT_FurnaceFuel.DT_FurnaceFuel" _array_element_2)
              (:then
                (if (== (.DA_Item (Utilities|Struct|BreakS_Fuel _returnvalue_2)) (.da_item _output_3))
                  (bind _output_get_2 (Variables|Default|SetCurrentFuel _returnvalue_2))
                  (Variables|Default|SetMaxFuelTime (.fueltime _output_get_2)))))))))
    (:then_2
      (Variables|Default|SetCurrentFuelTime (Utilities|Array|Get(acopy) _floats))
      (Variables|Default|SetCurrentCookTime (Utilities|Array|Get(acopy) _floats 1))
      (Actor|Tick|SetActorTickEnabled (Utilities|Array|Get(acopy) _booleans)))))

(fn CheckFreeBuildingPlacing
  (bind _returnvalue (Transformation|GetActorLocation))
  (bind (_valid _uniquefloors) (CallFunction|CornersTraces "(X=10.000000,Y=10.000000)" false))
  (if _valid
    (bind _returnvalue_2 (Collision|BoxTraceByChannel (+ _returnvalue "0,0,6.000000") (+ _returnvalue "0.000000,0.000000,70.000000") "40.000000,40.000000,1.000000" (Transformation|GetActorRotation) "TraceTypeQuery1" false 0 "None" true "(R=1.000000,G=0.000000,B=0.000000,A=1.000000)" "(R=0.000000,G=1.000000,B=0.000000,A=1.000000)" 2.0))
    (if (not _returnvalue_2)
      (return true (Utilities|Array|Get(acopy) _uniquefloors))
      (else
        (return false 0)))))

(fn HasFuel
  (bind (_array_element _array_index) (Utilities|Array|ForEachLoopwithBreak (Variables|/Script/SkyCraft.Inventory|GetSlots (Variables|Default|GetInventoryFuel)))
    (:LoopBody
      (Utilities|IsValid (.DA_Item (Utilities|Struct|BreakSlot _array_element))
        (:Is%20Valid
          (bind _outrownames (DataTable|GetDataTableRowNames "/Game/Blueprints/BuildingSystem/Furnace/DT_FurnaceFuel.DT_FurnaceFuel"))
          (bind _array_element_2 (Utilities|Array|ForEachLoopwithBreak _outrownames)
            (:LoopBody
              (bind _returnvalue (Utilities|GetDataTableRow "/Game/Blueprints/BuildingSystem/Furnace/DT_FurnaceFuel.DT_FurnaceFuel" _array_element_2)
                (:then
                  (if (== (.DA_Item (Utilities|Struct|BreakS_Fuel _returnvalue)) (.DA_Item (Utilities|Struct|BreakSlot _array_element)))
                    (return true _array_index _returnvalue)))))))))
    (:Completed
      (return false -1 ""))))

(fn ConsumeFuel
  (params (FuelIndex :type Integer) (S_Fuel :type S%20Fuel%20Structure))
  (bind _inventoryfuel (Variables|Default|GetInventoryFuel))
  (bind _inventoryfuel_2 (Variables|Default|GetInventoryFuel))
  (bind _slots (Variables|/Script/SkyCraft.Inventory|GetSlots _inventoryfuel))
  (bind _slots_2 (Variables|/Script/SkyCraft.Inventory|GetSlots _inventoryfuel_2))
  (bind _output (Utilities|Array|Get(acopy) _slots FuelIndex))
  (bind _output_2 (Utilities|Array|Get(acopy) _slots_2 FuelIndex))
  (bind _quantity (Utilities|Struct|BreakSlot _output))
  (bind _returnvalue (- _quantity 1))
  (bind _output_get (Variables|Default|SetCurrentFuel S_Fuel))
  (bind _output_get_2 (Variables|Default|SetCurrentFuelTime (.fueltime _output_get)))
  (Variables|Default|SetMaxFuelTime _output_get_2)
  (if (<= _returnvalue 0)
    (Class|Inventory|MulticastEmptySlot (Variables|Default|GetInventoryFuel) FuelIndex)
    (else
      (Class|Inventory|MulticastChangeSlot (Variables|Default|GetInventoryFuel) FuelIndex (Utilities|Struct|MakeSlot (.da_item _output_2) _returnvalue (.properties _output_2))))))

(fn ConsumeInput
  (params (S_FurnaceOutput :type S%20Furnace%20Output%20Structure))
  (bind _inventoryinput (Variables|Default|GetInventoryInput))
  (bind _inventoryinput_2 (Variables|Default|GetInventoryInput))
  (bind _inventoryoutput (Variables|Default|GetInventoryOutput))
  (bind _slots (Variables|/Script/SkyCraft.Inventory|GetSlots _inventoryinput))
  (bind _slots_2 (Variables|/Script/SkyCraft.Inventory|GetSlots _inventoryinput_2))
  (bind _slots_3 (Variables|/Script/SkyCraft.Inventory|GetSlots _inventoryoutput))
  (bind _output (Utilities|Array|Get(acopy) _slots))
  (bind _output_2 (Utilities|Array|Get(acopy) _slots_3))
  (bind _output_3 (Utilities|Array|Get(acopy) _slots_2))
  (bind _returnvalue (- (.quantity _output) 1))
  (Utilities|IsValid (.da_item _output_2)
    (:Is%20Valid
      (if (== (.da_item (.Output (Utilities|Struct|BreakS_FurnaceOutput S_FurnaceOutput))) (.da_item _output_2))
        (if (< (.quantity _output_2) (Variables|/Script/SkyCraft.DA_Item|GetMaxQuantity (.da_item _output_2)))
          (bind _output_get (Variables|Default|SetCurrentOutput S_FurnaceOutput :!label _label))
          (Variables|Default|SetMaxCookTime (.cooktime _output_get))
          (CallFunction|SetNoSpace false)
          (if (<= _returnvalue 0)
            (Class|Inventory|MulticastEmptySlot (Variables|Default|GetInventoryInput))
            (else
              (Class|Inventory|MulticastChangeSlot (Variables|Default|GetInventoryInput) 0 (Utilities|Struct|MakeSlot (.da_item _output_3) _returnvalue (.properties _output_3)))))
          (else
            (CallFunction|SetNoSpace true :!label _label_2)))
        (else
          (goto _label_2))))
    (:Is%20Not%20Valid
      (goto _label))))

(fn IsInputValid
  (Utilities|IsValid (.da_item (Utilities|Array|Get(acopy) (Variables|/Script/SkyCraft.Inventory|GetSlots (Variables|Default|GetInventoryInput))))
    (:Is%20Valid
      (bind _outrownames (DataTable|GetDataTableRowNames "/Game/Blueprints/BuildingSystem/Furnace/DT_FurnaceOutput.DT_FurnaceOutput"))
      (for _array_element _outrownames
        (bind _returnvalue (Utilities|GetDataTableRow "/Game/Blueprints/BuildingSystem/Furnace/DT_FurnaceOutput.DT_FurnaceOutput" _array_element)
          (:then
            (if (== (.DA_Item (Utilities|Struct|BreakSlot (.Input (Utilities|Struct|BreakS_FurnaceOutput _returnvalue)))) (.da_item (Utilities|Array|Get(acopy) (Variables|/Script/SkyCraft.Inventory|GetSlots (Variables|Default|GetInventoryInput)))))
              (return true _returnvalue)))))
      (CallFunction|SetNoSpace false)
      (return false ""))
    (:Is%20Not%20Valid
      (CallFunction|SetNoSpace false)
      (return false ""))))

(fn SetNoSpace
  (params (NoSpace :type Boolean))
  (if NoSpace
    (if (not (Variables|Default|GetNoSpace))
      (Variables|Default|SetNoSpace true))
    (elif (Variables|Default|GetNoSpace)
      (Variables|Default|SetNoSpace false))))

(fn OnFuel
  (Utilities|IsValid (.da_item (Variables|Default|GetCurrentFuel)) ; CurrentFuel
    (:Is%20Valid
      (Actor|Tick|SetActorTickEnabled true))
    (:Is%20Not%20Valid
      (bind (_has _index _s_fuel) (CallFunction|HasFuel))
      (if _has
        (Utilities|IsValid (.da_item (.output (Variables|Default|GetCurrentOutput))) ; CurrentOutput
          (:Is%20Valid
            (CallFunction|ConsumeFuel _index _s_fuel)
            (Actor|Tick|SetActorTickEnabled true))
          (:Is%20Not%20Valid
            (bind (_valid _s_furnaceoutput) (CallFunction|IsInputValid))
            (if _valid
              (CallFunction|ConsumeInput _s_furnaceoutput))))
        (else
          (Utilities|IsValid (.da_item (Utilities|Array|Get(acopy) (Variables|/Script/SkyCraft.Inventory|GetSlots (Variables|Default|GetInventoryInput))))
            (:Is%20Not%20Valid
              (CallFunction|SetNoSpace false))))))))

(fn DropItems
  (bind _inventoryinput (Variables|Default|GetInventoryInput))
  (bind _currentoutput (Variables|Default|GetCurrentOutput))
  (bind _inventoryoutput (Variables|Default|GetInventoryOutput))
  (bind _slots (Variables|/Script/SkyCraft.Inventory|GetSlots _inventoryoutput))
  (bind _slots_2 (Variables|/Script/SkyCraft.Inventory|GetSlots _inventoryinput))
  (bind _output (Utilities|Array|Get(acopy) _slots_2))
  (bind _output_2 (Utilities|Array|Get(acopy) _slots))
  (LocalVariables|Set_RootActorIsland (Class|AdianFL|GetRootActor self))
  (Utilities|FlowControl|Sequence
    (:then_0
      (Utilities|IsValid (.DA_Item (Utilities|Struct|BreakSlot _output))
        (:Is%20Valid
          (Game|SpawnActorfromClass "/Script/SkyCraft.DroppedItem" (Math|Transform|MakeTransform (Variables|/Script/Engine.SceneComponent|GetRelativeLocation (Variables|Transformation|GetRootComponent)) "0, 0, 0" "1.000000,1.000000,1.000000") "AlwaysSpawn" "MultiplyWithRoot" 0 (LocalVariables|Get_RootActorIsland) _output "RandomDirection" "0.000000,0.000000,0.000000" (LocalVariables|Get_RandomMagnitude) 0 0))))
    (:then_1
      (Utilities|IsValid (.DA_Item (Utilities|Struct|BreakSlot _output_2))
        (:Is%20Valid
          (Game|SpawnActorfromClass "/Script/SkyCraft.DroppedItem" (Math|Transform|MakeTransform (Variables|/Script/Engine.SceneComponent|GetRelativeLocation (Variables|Transformation|GetRootComponent)) "0, 0, 0" "1.000000,1.000000,1.000000") "AlwaysSpawn" "MultiplyWithRoot" 0 (LocalVariables|Get_RootActorIsland) _output_2 "RandomDirection" "0.000000,0.000000,0.000000" (LocalVariables|Get_RandomMagnitude) 0 0))))
    (:then_2
      (for _array_element (Variables|/Script/SkyCraft.Inventory|GetSlots (Variables|Default|GetInventoryFuel))
        (Utilities|IsValid (.DA_Item (Utilities|Struct|BreakSlot _array_element))
          (:Is%20Valid
            (Game|SpawnActorfromClass "/Script/SkyCraft.DroppedItem" (Math|Transform|MakeTransform (Variables|/Script/Engine.SceneComponent|GetRelativeLocation (Variables|Transformation|GetRootComponent)) "0, 0, 0" "1.000000,1.000000,1.000000") "AlwaysSpawn" "MultiplyWithRoot" 0 (LocalVariables|Get_RootActorIsland) _array_element "RandomDirection" "0.000000,0.000000,0.000000" (LocalVariables|Get_RandomMagnitude) 0 0)))))
    (:then_3
      (Utilities|IsValid (.DA_Item (Utilities|Struct|BreakSlot (.input _currentoutput)))
        (:Is%20Valid
          (Game|SpawnActorfromClass "/Script/SkyCraft.DroppedItem" (Math|Transform|MakeTransform (Variables|/Script/Engine.SceneComponent|GetRelativeLocation (Variables|Transformation|GetRootComponent)) "0, 0, 0" "1.000000,1.000000,1.000000") "AlwaysSpawn" "MultiplyWithRoot" 0 (LocalVariables|Get_RootActorIsland) (.input _currentoutput) "RandomDirection" "0.000000,0.000000,0.000000" (LocalVariables|Get_RandomMagnitude) 0 0))))))

(fn OnRepCurrentFuelTime
  (Variables|Default|SetLastFuelTime (Variables|Default|GetCurrentFuelTime))
  (Variables|Default|SetLastUpdateFuelTime (Utilities|Time|GetGameTimeinSeconds)))

(fn OnRepCurrentOutput
  (Default|CallOnCurrentOutput))

(fn OnRepCurrentFuel
  (Default|CallOnCurrentFuel)
  (Rendering|SetVisibility (Variables|Default|GetPointLight) (Utilities|IsValid (.da_item (Variables|Default|GetCurrentFuel))) false))

(fn CornersTraces
  (params (Dimensions :type Vector%202D%20Structure) (Debug :type Boolean))
  (bind (_valid _uniquefloors) (|CallParentFunction "(X=70.000000,Y=70.000000)" false))
  (return _valid _uniquefloors))

(fn ClientInteractBP
  (params (InteractKey :type EInteractKey%20Enum :default "Interact1") (Pawn :type Pawn%20Object%20Reference) (BP_PSS :type BP%20PSS%20Object%20Reference))
  (switch Utilities|FlowControl|Switch|SwitchonEInteractKey InteractKey
    (:Interact1
      (bind _returnvalue (UserInterface|CreateWidget "/Game/Widgets/CWS/CWS_Furnace.CWS_Furnace_C" 0 self))
      (UserInterface|Viewport|AddtoViewport _returnvalue 50)
      (Default|AddCWS BP_PSS _returnvalue true true true "NewEnumerator2")
      (return true))))

(fn ClientInterruptBP
  (params (InterruptedBy :type EInterruptedBy%20Enum :default "Player") (InteractKey :type EInteractKey%20Enum :default "Interact1") (Pawn :type Pawn%20Object%20Reference) (BP_PSS :type BP%20PSS%20Object%20Reference))
  (return false))

(fn ServerInteractBP
  (params (InteractKey :type EInteractKey%20Enum :default "Interact1") (Pawn :type Pawn%20Object%20Reference) (BP_PSS :type BP%20PSS%20Object%20Reference))
  (return false))

(fn ServerInterruptBP
  (params (InterruptedBy :type EInterruptedBy%20Enum :default "Player") (InteractKey :type EInteractKey%20Enum :default "Interact1") (Pawn :type Pawn%20Object%20Reference) (BP_PSS :type BP%20PSS%20Object%20Reference))
  (return false))