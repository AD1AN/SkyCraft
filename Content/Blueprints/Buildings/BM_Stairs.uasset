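; Stairs building piece that supplies its own placement checks on top of a parent building class.
; Both checks run the same Visibility box sweep, pitched along the stair slope and offset from the actor.
; BodyTraces passes when the sweep hits nothing or an Island.
; GroundTraces passes only when it hits the given island and that actor carries the Island sky tag.
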(fn ConstructionScript
  (|CallParentFunction))

(fn BodyTraces
  (bind _returnvalue (Transformation|GetActorRotation))
  (bind (_outhit _returnvalue_2) (Collision|BoxTraceByChannel (CallFunction|OffsettedLocation "125.000000,0.000000,-15.000000") (CallFunction|OffsettedLocation "-90.000000,0.000000,-120.000000") "5.000000,130.000000,10.000000" (Math|Rotator|MakeRotator (.roll _returnvalue) 26.5 (.yaw _returnvalue)) "TraceTypeQuery1" false 0 "None" true "(R=1.000000,G=0.000000,B=0.000000,A=1.000000)" "(R=0.000000,G=1.000000,B=0.000000,A=1.000000)" 2.0))
  (if _returnvalue_2
    (return (Class|GameplayStatics|ObjectIsA (.HitActor (Collision|BreakHitResult _outhit)) "/Script/SkyCraft.Island"))
    (else
      (return true))))

(fn GroundTraces
  (params (Island :type Actor%20Object%20Reference))
  (bind _returnvalue (Transformation|GetActorRotation))
  (bind (_outhit _returnvalue_2) (Collision|BoxTraceByChannel (CallFunction|OffsettedLocation "125.000000,0.000000,-15.000000") (CallFunction|OffsettedLocation "-90.000000,0.000000,-120.000000") "5.000000,130.000000,10.000000" (Math|Rotator|MakeRotator (.roll _returnvalue) 26.5 (.yaw _returnvalue)) "TraceTypeQuery1" false 0 "None" true "(R=1.000000,G=0.000000,B=0.000000,A=1.000000)" "(R=0.000000,G=1.000000,B=0.000000,A=1.000000)" 2.0))
  (if _returnvalue_2
    (if (Class|AdianFL|ActorHasSkyTag (.HitActor (Collision|BreakHitResult _outhit)) "/Game/DataAssets/SkyTag/Island.Island")
      (return (== (.HitActor (Collision|BreakHitResult _outhit)) Island)))
    (else
      (return false))))