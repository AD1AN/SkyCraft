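; Foundation building piece that supplies placement checks for whether it can sit on an Island.
; BodyTraces passes only when a thin, rotated box trace at the actor's location hits nothing on Visibility.
; GridTraces casts small boxes downward near the four corners and requires every one to hit an Island, returning validity and that Island.
; An alternative check accepting foundation-tagged actors as support is present but unused.
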(fn ConstructionScript)

(fn BodyTraces
  (bind _returnvalue (Transformation|GetActorLocation))
  (bind _returnvalue_2 (Collision|BoxTraceByChannel _returnvalue _returnvalue "130.000000,130.000000,3.000000" (Transformation|GetActorRotation) "TraceTypeQuery1" false 0 "None" true "(R=1.000000,G=0.000000,B=0.000000,A=1.000000)" "(R=0.000000,G=1.000000,B=0.000000,A=1.000000)" 2.0))
  (return (not _returnvalue_2)))

(fn GridTraces
  (bind (_outhit _returnvalue) (Collision|BoxTraceByChannel (CallFunction|OffsettedLocation "125.000000,125.000000,-15.000000") (CallFunction|OffsettedLocation "125.000000,125.000000,-280.000000") "15.000000,15.000000,10.000000" (Transformation|GetActorRotation) "TraceTypeQuery1" false 0 "None" true "(R=1.000000,G=0.000000,B=0.000000,A=1.000000)" "(R=0.000000,G=1.000000,B=0.000000,A=1.000000)" 2.0))
  (bind (_outhit_2 _returnvalue_2) (Collision|BoxTraceByChannel (CallFunction|OffsettedLocation "-125.000000,-125.000000,-15.000000") (CallFunction|OffsettedLocation "-125.000000,-125.000000,-280.000000") "15.000000,15.000000,10.000000" (Transformation|GetActorRotation) "TraceTypeQuery1" false 0 "None" true "(R=1.000000,G=0.000000,B=0.000000,A=1.000000)" "(R=0.000000,G=1.000000,B=0.000000,A=1.000000)" 2.0))
  (bind (_outhit_3 _returnvalue_3) (Collision|BoxTraceByChannel (CallFunction|OffsettedLocation "125.000000,-125.000000,-15.000000") (CallFunction|OffsettedLocation "125.000000,-125.000000,-280.000000") "15.000000,15.000000,10.000000" (Transformation|GetActorRotation) "TraceTypeQuery1" false 0 "None" true "(R=1.000000,G=0.000000,B=0.000000,A=1.000000)" "(R=0.000000,G=1.000000,B=0.000000,A=1.000000)" 2.0))
  (bind (_outhit_4 _returnvalue_4) (Collision|BoxTraceByChannel (CallFunction|OffsettedLocation "-125.000000,125.000000,-15.000000") (CallFunction|OffsettedLocation "-125.000000,125.000000,-280.000000") "15.000000,15.000000,10.000000" (Transformation|GetActorRotation) "TraceTypeQuery1" false 0 "None" true "(R=1.000000,G=0.000000,B=0.000000,A=1.000000)" "(R=0.000000,G=1.000000,B=0.000000,A=1.000000)" 2.0))
  (if (Math|Boolean|ANDBoolean _returnvalue_4 _returnvalue_3 _returnvalue_2 _returnvalue)
    (if (Math|Boolean|ANDBoolean (Class|GameplayStatics|ObjectIsA (.HitActor (Collision|BreakHitResult _outhit)) "/Script/SkyCraft.Island") (Class|GameplayStatics|ObjectIsA (.HitActor (Collision|BreakHitResult _outhit_2)) "/Script/SkyCraft.Island") (Class|GameplayStatics|ObjectIsA (.HitActor (Collision|BreakHitResult _outhit_3)) "/Script/SkyCraft.Island") (Class|GameplayStatics|ObjectIsA (.HitActor (Collision|BreakHitResult _outhit_4)) "/Script/SkyCraft.Island"))
      (bind _asisland (Utilities|Casting|CastToIsland (.HitActor (Collision|BreakHitResult _outhit_4)))
        (:then
          (return true _asisland))
        (:CastFailed
          _))))
  (return false 0))