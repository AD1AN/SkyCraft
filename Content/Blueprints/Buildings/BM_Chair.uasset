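; BM_Chair is a chair building Blueprint that defines the clearance check for the space its body occupies.
; BodyTraces sweeps two downward box traces on the Visibility channel, aligned to the actor's rotation: a wide, low one at the center and a thin, taller one offset along local X.
; It returns true only when neither trace hits, approximating the chair's shape with two volumes.
; The construction script is empty.
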(fn ConstructionScript)

(fn BodyTraces
  (bind _returnvalue (Collision|BoxTraceByChannel (CallFunction|OffsettedLocation "0.000000,0.000000,63.000000") (CallFunction|OffsettedLocation "0.000000,0.000000,10.000000") "20.000000,20.000000,1.000000" (Transformation|GetActorRotation) "TraceTypeQuery1" false 0 "None"))
  (bind _returnvalue_2 (Collision|BoxTraceByChannel (CallFunction|OffsettedLocation "25.000000,0.000000,120.000000") (CallFunction|OffsettedLocation "25.000000,0.000000,10.000000") "3.000000,20.000000,1.000000" (Transformation|GetActorRotation) "TraceTypeQuery1" false 0 "None"))
  (return (and (not _returnvalue) (not _returnvalue_2))))