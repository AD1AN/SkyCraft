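; Workbench building, a child Blueprint that opens the workbench UI when a player interacts with it.
; Placement checks pass a fixed footprint to the parent corner traces and run a downward, rotation-aligned box trace that must hit nothing.
; The first interact key creates the CWS_Workbench widget client-side and registers it with BPPSS.
; Server interact and both interrupt handlers only return false.
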(fn ConstructionScript
  (|CallParentFunction))

(fn CornersTraces
  (params (Dimensions :type Vector%202D%20Structure) (Debug :type Boolean))
  (bind (_valid _uniquefloors) (|CallParentFunction "(X=70.000000,Y=140.000000)" false))
  (return _valid _uniquefloors))

(fn BodyTraces
  (bind _returnvalue (Collision|BoxTraceByChannel (CallFunction|OffsettedLocation "-10.000000,0.000000,120.000000") (CallFunction|OffsettedLocation "-10.000000,0.000000,20.000000") "40.000000,70.000000,1.000000" (Transformation|GetActorRotation) "TraceTypeQuery1" false 0 "None" true "(R=1.000000,G=0.000000,B=0.000000,A=1.000000)" "(R=0.000000,G=1.000000,B=0.000000,A=1.000000)" 2.0))
  (return (not _returnvalue)))

(fn ClientInteractBP
  (params (InteractKey :type EInteractKey%20Enum :default "Interact1") (Pawn :type Pawn%20Object%20Reference) (BP_PSS :type BP%20PSS%20Object%20Reference))
  (switch Utilities|FlowControl|Switch|SwitchonEInteractKey InteractKey
    (:Interact1
      (bind _returnvalue (UserInterface|CreateWidget "/Game/Widgets/CWS/CWS_Workbench.CWS_Workbench_C"))
      (UserInterface|Viewport|AddtoViewport _returnvalue 25)
      (Default|AddCWS BP_PSS _returnvalue true true true "NewEnumerator2")
      (return true))))

(fn ClientInterruptBP
  (params (InterruptedBy :type EInterruptedBy%20Enum :default "Player") (InteractKey :type EInteractKey%20Enum :default "Interact1") (Pawn :type Pawn%20Object%20Reference) (BP_PSS :type BP%20PSS%20Object%20Reference))
  (return false))

(fn ServerInteractBP
  (params (InteractKey :type EInteractKey%20Enum :default "Interact1") (Pawn :type Pawn%20Object%20Reference) (BP_PSS :type BP%20PSS%20Object%20Reference))
  (return false))

(fn ServerInterruptBP
  (params (InterruptedBy :type EInterruptedBy%20Enum :default "Player") (InteractKey :type EInteractKey%20Enum :default "Interact1") (Pawn :type Pawn%20Object%20Reference) (BP_PSS :type BP%20PSS%20Object%20Reference))
  (return false))