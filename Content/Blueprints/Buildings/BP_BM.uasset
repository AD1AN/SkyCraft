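; BP_BM is a building actor with helpers for placement validation and preview.
; CornersTraces line-traces vertically at the four rotated footprint corners, passing only if all hit Building-tagged actors or all hit Islands, and returns the unique floors.
; PreviewMode caches each static mesh's materials to swap in a preview material and restore them later, alongside collision-toggle and local-offset helpers.
; Body, ground and grid checks are stubs that always pass.
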(fn ConstructionScript
  (PreviewTraces|CornersTraces "(X=15.000000,Y=15.000000)" false))

(fn BodyTraces
  (return true))

(fn GroundTraces
  (params (Island :type Actor%20Object%20Reference))
  (return true))

(fn GridTraces
  (return true 0))

(fn CornersTraces
  (params (Dimensions :type Vector%202D%20Structure :default "(X=10.000000,Y=10.000000)") (Debug :type Boolean))
  (bind _returnvalue (Transformation|GetActorLocation))
  (bind _returnvalue_2 (Transformation|GetActorRotation))
  (bind _returnvalue_3 (/ (.x Dimensions) 2.0))
  (bind _returnvalue_4 (/ (.y Dimensions) 2.0))
  (bind __uniquefloors (LocalVariables|Get_UniqueFloors))
  (bind _returnvalue_5 (Math|Vector|GetRightVector _returnvalue_2))
  (bind _returnvalue_6 (Math|Vector|GetForwardVector _returnvalue_2))
  (bind _returnvalue_7 (+ _returnvalue "0,0,5.000000"))
  (bind _returnvalue_8 (select Debug "ForOneFrame" "None"))
  (bind _returnvalue_9 (* _returnvalue_4 _returnvalue_5 -1.0))
  (bind _returnvalue_10 (* _returnvalue_3 _returnvalue_6 -1.0))
  (bind _returnvalue_11 (* _returnvalue_3 _returnvalue_6))
  (bind _returnvalue_12 (* _returnvalue_4 _returnvalue_5))
  (bind _returnvalue_13 (+ _returnvalue_11 _returnvalue_12 _returnvalue_7))
  (bind _returnvalue_14 (+ _returnvalue_11 _returnvalue_9 _returnvalue_7))
  (bind _returnvalue_15 (+ _returnvalue_10 _returnvalue_9 _returnvalue_7))
  (bind _returnvalue_16 (+ _returnvalue_10 _returnvalue_12 _returnvalue_7))
  (bind _outhit (Collision|LineTraceByChannel (+ _returnvalue_13 "0.000000,0.000000,25.000000") (+ _returnvalue_13 "0.000000,0.000000,-25.000000") "TraceTypeQuery1" false 0 _returnvalue_8))
  (bind _outhit_2 (Collision|LineTraceByChannel (+ _returnvalue_14 "0.000000,0.000000,25.000000") (+ _returnvalue_14 "0.000000,0.000000,-25.000000") "TraceTypeQuery1" false 0 _returnvalue_8))
  (bind _outhit_3 (Collision|LineTraceByChannel (+ _returnvalue_15 "0.000000,0.000000,25.000000") (+ _returnvalue_15 "0.000000,0.000000,-25.000000") "TraceTypeQuery1" false 0 _returnvalue_8))
  (bind _outhit_4 (Collision|LineTraceByChannel (+ _returnvalue_16 "0.000000,0.000000,25.000000") (+ _returnvalue_16 "0.000000,0.000000,-25.000000") "TraceTypeQuery1" false 0 _returnvalue_8))
  (Utilities|Array|AddUnique __uniquefloors (.HitActor (Collision|BreakHitResult _outhit_2)))
  (Utilities|Array|AddUnique __uniquefloors (.HitActor (Collision|BreakHitResult _outhit)))
  (Utilities|Array|AddUnique __uniquefloors (.HitActor (Collision|BreakHitResult _outhit_3)))
  (Utilities|Array|AddUnique __uniquefloors (.HitActor (Collision|BreakHitResult _outhit_4)))
  (if (Math|Boolean|ANDBoolean (Class|AdianFL|ActorHasSkyTag (.HitActor (Collision|BreakHitResult _outhit_2)) "/Game/DataAssets/SkyTag/Building.Building") (Class|AdianFL|ActorHasSkyTag (.HitActor (Collision|BreakHitResult _outhit)) "/Game/DataAssets/SkyTag/Building.Building") (Class|AdianFL|ActorHasSkyTag (.HitActor (Collision|BreakHitResult _outhit_3)) "/Game/DataAssets/SkyTag/Building.Building") (Class|AdianFL|ActorHasSkyTag (.HitActor (Collision|BreakHitResult _outhit_4)) "/Game/DataAssets/SkyTag/Building.Building"))
    (return true (LocalVariables|Get_UniqueFloors))
    (elif (Math|Boolean|ANDBoolean (Class|GameplayStatics|ObjectIsA (.HitActor (Collision|BreakHitResult _outhit_2)) "/Script/SkyCraft.Island") (Class|GameplayStatics|ObjectIsA (.HitActor (Collision|BreakHitResult _outhit)) "/Script/SkyCraft.Island") (Class|GameplayStatics|ObjectIsA (.HitActor (Collision|BreakHitResult _outhit_3)) "/Script/SkyCraft.Island") (Class|GameplayStatics|ObjectIsA (.HitActor (Collision|BreakHitResult _outhit_4)) "/Script/SkyCraft.Island"))
      (return true (LocalVariables|Get_UniqueFloors))
      (else
        (return false 0)))))

(fn PreviewMode
  (params (PreviewMode :type Boolean))
  (if PreviewMode
    (bind _output_get (LocalVariables|Set_StaticMeshes (Actor|GetComponentsByClass "/Script/Engine.StaticMeshComponent")))
    (for _array_element _output_get
      (Utilities|Map|Add (Variables|Default|GetStoredMaterials) _array_element (Utilities|Struct|MakeArrayMaterials (Rendering|Material|GetMaterials _array_element)))
      (for (_ _array_index) (Rendering|Material|GetMaterials _array_element)
        (Rendering|Material|SetMaterial _array_element _array_index "/Game/Materials/M_BuildingPreview.M_BuildingPreview")))
    (else
      (bind _keys (Utilities|Map|Keys (Variables|Default|GetStoredMaterials)))
      (for _array_element_2 _keys
        (for (_array_element_3 _array_index_2) (.materials (.Value (Utilities|Map|Find (Variables|Default|GetStoredMaterials) _array_element_2)))
          (Rendering|Material|SetMaterial _array_element_2 _array_index_2 _array_element_3))))))

(fn CollisionMode
  (params (Enabled :type Boolean))
  (Collision|SetActorEnableCollision Enabled))

(fn OffsettedLocation
  (params (Offset :type Vector))
  (return (Math|Transform|TransformLocation (Transformation|GetActorTransform) Offset)))