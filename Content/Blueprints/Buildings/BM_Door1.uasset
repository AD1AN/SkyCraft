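; Hinged door building that players open and close through the interact system, with its open state saved and loaded.
; Server interaction, ignored mid-swing, multicasts the toggle to a timeline that yaws the mesh up to 90 degrees, with authority setting Opened on finish.
; Opened's RepNotify updates the Open/Close prompt and snaps the timeline when not animating.
; BodyTraces uses a box trace to report whether the door's space is unobstructed.
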(event Custom|Multicast_ToggleDoor
  (params (Open :type Boolean))
  (Variables|Default|SetAnimated true)
  (if Open
    (bind _newtrack_0 (Timeline|Timeline Play)
      (:Update
        (Transformation|SetRelativeRotation (Variables|Default|GetStaticMesh) (Math|Rotator|MakeRotator 0.0 0.0 (Math|Float|Lerp 0.0 9e+01 _newtrack_0)) false false))
      (:Finished
        (Variables|Default|SetAnimated false)
        (Networking|SwitchHasAuthority
          (:Authority
            (Variables|Default|SetOpened Open)))))
    (else
      (Timeline|Timeline Reverse))))

(fn ConstructionScript
  (|CallParentFunction))

(fn OnRepOpened
  (Class|InteractComponent|TextChange (Variables|Default|GetInteractSystem) (select (Variables|Default|GetOpened) "Close" "Open"))
  (Networking|ForceNetUpdate)
  (if (not (Variables|Default|GetAnimated))
    (Components|Timeline|SetNewTime (Variables|Default|GetTimeline) (select (Variables|Default|GetOpened) 0.5 0.0))))

(fn BodyTraces
  (bind _returnvalue (Collision|BoxTraceByChannel (CallFunction|OffsettedLocation "0.000000,-66.599998,90.000000") (CallFunction|OffsettedLocation "0.000000,-66.599998,-80.000000") "5.000000,60.000000,5.000000" (Transformation|GetActorRotation) "TraceTypeQuery1" false 0 "None" true "(R=1.000000,G=0.000000,B=0.000000,A=1.000000)" "(R=0.000000,G=1.000000,B=0.000000,A=1.000000)" 2.0))
  (return (not _returnvalue)))

(fn SaveBuildingParameters
  (return (Utilities|Struct|MakeBuildingParameters 0 0 0 0 0 0 0 0 (Utilities|Array|MakeArray (Variables|Default|GetOpened)))))

(fn LoadBuildingParameters
  (params (BuildingParameters :type Building%20Parameters%20Structure))
  (Variables|Default|SetOpened (Utilities|Array|Get(acopy) (.Booleans (Utilities|Struct|BreakBuildingParameters BuildingParameters))))
  (return true))

(fn ClientInteractBP
  (params (InteractKey :type EInteractKey%20Enum :default "Interact1") (Pawn :type Pawn%20Object%20Reference) (BP_PSS :type BP%20PSS%20Object%20Reference))
  (return false))

(fn ClientInterruptBP
  (params (InterruptedBy :type EInterruptedBy%20Enum :default "Player") (InteractKey :type EInteractKey%20Enum :default "Interact1") (Pawn :type Pawn%20Object%20Reference) (BP_PSS :type BP%20PSS%20Object%20Reference))
  (return false))

(fn ServerInteractBP
  (params (InteractKey :type EInteractKey%20Enum :default "Interact1") (Pawn :type Pawn%20Object%20Reference) (BP_PSS :type BP%20PSS%20Object%20Reference))
  (if (not (Variables|Default|GetAnimated))
    (CallFunction|MulticastToggleDoor (not (Variables|Default|GetOpened)))
    (return true)))

(fn ServerInterruptBP
  (params (InterruptedBy :type EInterruptedBy%20Enum :default "Player") (InteractKey :type EInteractKey%20Enum :default "Interact1") (Pawn :type Pawn%20Object%20Reference) (BP_PSS :type BP%20PSS%20Object%20Reference))
  (return false))