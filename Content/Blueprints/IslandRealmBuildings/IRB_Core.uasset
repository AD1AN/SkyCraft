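; IRB_Core is a base Blueprint for Island Realm buildings that exposes a common interaction contract.
; Client and server interact and interrupt hooks receive the key and pawn, and all return false by default, apparently as stubs for child buildings to override.
; Getters supply the InteractSystem reference and use the actor's location as the interaction point.
; The construction script is empty.
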(fn ConstructionScript)

(fn ClientInteractBP
  (params (InteractKey :type EInteractKey%20Enum :default "Interact1") (Pawn :type Pawn%20Object%20Reference) (BP_PAI :type BP%20PAI%20Object%20Reference))
  (return false))

(fn ClientInterruptBP
  (params (InterruptedBy :type EInterruptedBy%20Enum :default "Player") (InteractKey :type EInteractKey%20Enum :default "Interact1") (Pawn :type Pawn%20Object%20Reference) (BP_PAI :type BP%20PAI%20Object%20Reference))
  (return false))

(fn GetInteractLocation
  (return (Transformation|GetActorLocation)))

(fn GetInteractSystem
  (return (Variables|Default|GetInteractSystem)))

(fn ServerInteractBP
  (params (InteractKey :type EInteractKey%20Enum :default "Interact1") (Pawn :type Pawn%20Object%20Reference) (BP_PAI :type BP%20PAI%20Object%20Reference))
  (return false))

(fn ServerInterruptBP
  (params (InterruptedBy :type EInterruptedBy%20Enum :default "Player") (InteractKey :type EInteractKey%20Enum :default "Interact1") (Pawn :type Pawn%20Object%20Reference) (BP_PAI :type BP%20PAI%20Object%20Reference))
  (return false))