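; Player form pawn for the Crystal state, with orbit look, island menu and inventory, from which the player revives.
; Holding Jump fills a progress bar, then the server spawns PF_Normal at a traced spot if the island IsCrystal, otherwise an estray PF_Phantom.
; A multicast spline timeline animates the spirit, Niagara effect and blur before the server possesses the new pawn and destroys this one.
; It also handles entering Astral behind a black screen.
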(event Custom|ShowCompleted)

(event Custom|Client_SetRandomRotation
  (bind _returnvalue (Math|Random|RandomFloatinRange 5.0 355.0))
  (Pawn|SetControlRotation (Variables|Default|GetBP_PCS) (Math|Rotator|MakeRotator 0.0 0.0 _returnvalue)) ; If rotation default = wind sound is freaking
  (Transformation|SetWorldRotation (Variables|Default|GetSkySpringArmComponent) (Math|Rotator|MakeRotator 0.0 -2e+01 _returnvalue) false false))

(event Custom|OpenCompleted)

(event Custom|OnIsCrystal_Event
  (Transformation|SetRelativeLocation (Variables|Default|GetSkySpringArmComponent) (Math|Vector|MakeVector 0.0 0.0 (Math|Float|SelectFloat 5e+01 0.0 (Variables|/Script/SkyCraft.PlayerIsland|GetbIsCrystal (Variables|/Game/Blueprints/BP_PSS.BP_PSS_C|GetBP_PlayerIsland (Variables|Default|GetBP_PSS))))) false false))

(event Custom|Multicast_InitSetup
  (params (Inventory :type Array%20of%20Slot%20Structures) (Equipment :type Array%20of%20Slot%20Structures))
  (Variables|/Script/SkyCraft.InventoryComponent|SetSlots (Variables|Default|GetInventoryComponent) Inventory)
  (Variables|/Script/SkyCraft.InventoryComponent|SetSlots (Variables|Default|GetEquipmentInventoryComponent) Equipment))

(event Custom|OnDestroyed_Event_0
  (params (DestroyedActor :type Actor%20Object%20Reference))
  (if (Variables|Default|GetEmerging)
    _))

(event Input|EnhancedActionEvents|EnhancedInputActionInteract1
  (params (ActionValue :type Boolean) (ElapsedSeconds :type Float%20%28double-precision%29) (TriggeredSeconds :type Float%20%28double-precision%29) (InputAction :type Input%20Action%20Object%20Reference :default "/Game/Misc/EnhancedInput/Interact1.Interact1"))
  (bind _bp_pss (Variables|Default|GetBP_PSS))
  (:Started
    (Default|CreateMenu (Variables|/Game/Blueprints/BP_PSS.BP_PSS_C|GetBP_PlayerIsland _bp_pss) self _bp_pss)))

(event EventBeginPlay
  (bind _asbp_gss (Utilities|Casting|CastToBP_GSS (Game|GetGameState)))
  (Variables|Default|SetBP_GSS _asbp_gss)
  (bind _asbp_pcs (Utilities|Casting|CastToBP_PCS (Components|GetOwner))) ; Server&Owner
  (bind _output_get (Variables|Default|SetBP_PCS _asbp_pcs))
  (Variables|Default|SetBP_PSS (Variables|/Game/Blueprints/BP_PCS.BP_PCS_C|GetBP_PSS _output_get))
  (Utilities|FlowControl|Sequence
    (:then_0
      (Networking|SwitchHasAuthority
        (:Authority
          (bind _asbp_gms (Utilities|Casting|CastToBP_GMS (Game|GetGameMode)))
          (Variables|Default|SetBP_GMS _asbp_gms)
          (Game|AssignOnDestroyed (delegate Custom|OnDestroyed_Event_0)))))
    (:then_1
      (if (Class|PSS|IsLocalState (Variables|Default|GetBP_PSS))
        (Utilities|IsValid (Variables|/Game/Blueprints/BP_PSS.BP_PSS_C|GetBP_PlayerIsland (Variables|Default|GetBP_PSS))
          (:Is%20Valid
            (EventDispatchers|AssignOnIsCrystal (Variables|/Game/Blueprints/BP_PSS.BP_PSS_C|GetBP_PlayerIsland (Variables|Default|GetBP_PSS)) (delegate Custom|OnIsCrystal_Event))))))))

(event EventPossessed
  (params (NewController :type Controller%20Object%20Reference))
  (Default|MulticastPlayerFormPossessed (Variables|Default|GetBP_PSS) "Crystal" self)
  (Game|Player|SetViewTargetwithBlend (Variables|Default|GetBP_PCS) self 0.0 "VTBlend_Linear" 0.0 false))

(event EventClientPossessed
  (bind _bp_pcs (Variables|Default|GetBP_PCS))
  (bind _w_eyestransition (Variables|/Game/Blueprints/BP_PCS.BP_PCS_C|GetW_EyesTransition _bp_pcs))
  (Rendering|Material|SetScalarParameterValue "/Game/Materials/Col_Blur.Col_Blur" "BlurAmount" 0.3 :!class /Script/Engine.KismetMaterialLibrary)
  (bind _returnvalue (UserInterface|CreateWidget "/Game/Widgets/W_PF_Crystal.W_PF_Crystal_C" (Variables|Default|GetBP_PCS)))
  (bind _output_get (Variables|Default|SetW_PF_Island _returnvalue))
  (Default|ShowAnimation _output_get (delegate Custom|ShowCompleted))
  (UserInterface|Viewport|AddtoViewport _output_get 0)
  (Utilities|IsValid _w_eyestransition
    (:Is%20Valid
      (Default|OpenEyes _w_eyestransition (delegate Custom|OpenCompleted)))))

(event EventClientUnpossessed
  (Default|HideandRemove (Variables|Default|GetW_PF_Island)))

(event EventTick
  (params (DeltaSeconds :type Float%20%28single-precision%29)))

(event EventRestarted
  (if (Pawn|IsLocallyControlled)
    (Input|EnableInput (Variables|Default|GetBP_PCS))))

(event Custom|Server_SpawnNormal
  (params (Location :type Vector%20Net%20Quantize%20Structure) (YawRotation :type Float%20%28double-precision%29))
  (CallFunction|SpawnNormal Location YawRotation))

(event Custom|Multicast_StartSpawnDeadSpirit
  (params (YawRotation :type Float%20%28double-precision%29))
  (bind _spawned_pf_spirit (Variables|Default|GetSpawned_PF_Spirit))
  (Transformation|SetActorRotation (Math|Rotator|MakeRotator 0.0 0.0 YawRotation))
  (bind _returnvalue (Niagara|SpawnSystemAttached "/Game/Niagara/NS_IslandPhantomMesh.NS_IslandPhantomMesh" 0 "None" "0, 0, 0" "0, 0, 0" "KeepRelativeOffset" true true "AutoRelease")) ; It should not be attached to SpiritMesh, because "local".
  (Variables|Default|SetNS_IslandSpirit _returnvalue)
  (Rendering|SetVisibility (Variables|Default|GetSpiritMesh) true false)
  (bind _move (Timeline|Timeline PlayFromStart)
    (:Update
      (Transformation|SetRelativeLocation (Variables|Default|GetSpiritMesh) (Spline|GetLocationatDistanceAlongSpline (Variables|Default|GetSpline_Spirit) (Math|Float|Lerp 0.0 (Spline|GetSplineLength (Variables|Default|GetSpline_Spirit)) _move) "Local") false false)
      (Class|CameraComponent|SetPostProcessBlendWeight (Variables|Default|GetCamera) (- 1.0 _move))
      (Rendering|Material|SetScalarParameterValue "/Game/Materials/Col_Blur.Col_Blur" "BlurAmount" (Math|Float|Lerp 0.3 0.0 _move) :!class /Script/Engine.KismetMaterialLibrary)
      (Utilities|IsValid (Variables|Default|GetNS_IslandSpirit)
        (:Is%20Valid
          (Niagara|SetNiagaraVariable(Vector3) (Variables|Default|GetNS_IslandSpirit) "PivotLocation" (Variables|/Script/Engine.SceneComponent|GetRelativeLocation (Variables|Default|GetSpiritMesh)))
          (Niagara|SetNiagaraVariable(Float) (Variables|Default|GetNS_IslandSpirit) "Progress" _move))))
    (:Finished
      (Networking|SwitchHasAuthority
        (:Authority
          (Pawn|Possess (Variables|Default|GetBP_PCS) _spawned_pf_spirit)
          (Default|MulticastToggleVisibility _spawned_pf_spirit true)
          (Actor|DestroyActor))))))

(event Custom|Multicast_StartSpawnNormal
  (params (YawRotation :type Float%20%28double-precision%29))
  (Transformation|SetActorRotation (Math|Rotator|MakeRotator 0.0 0.0 YawRotation))
  (bind _returnvalue (Niagara|SpawnSystemAttached "/Game/Niagara/NS_IslandPhantomMesh.NS_IslandPhantomMesh" 0 "None" "0, 0, 0" "0, 0, 0" "KeepRelativeOffset" true true "AutoRelease")) ; It should not be attached to SpiritMesh, because "local".
  (Variables|Default|SetNS_IslandSpirit _returnvalue)
  (Rendering|SetVisibility (Variables|Default|GetSpiritMesh) true false)
  (bind _move (Timeline|TimelineSpawn PlayFromStart)
    (:Update
      (Transformation|SetRelativeLocation (Variables|Default|GetSpiritMesh) (Spline|GetLocationatDistanceAlongSpline (Variables|Default|GetSpline_Normal) (Math|Float|Lerp 0.0 (Spline|GetSplineLength (Variables|Default|GetSpline_Normal)) _move) "Local") false false)
      (Class|CameraComponent|SetPostProcessBlendWeight (Variables|Default|GetCamera) (- 1.0 _move))
      (Rendering|Material|SetScalarParameterValue "/Game/Materials/Col_Blur.Col_Blur" "BlurAmount" (Math|Float|Lerp 0.3 0.0 _move) :!class /Script/Engine.KismetMaterialLibrary)
      (Utilities|IsValid (Variables|Default|GetNS_IslandSpirit)
        (:Is%20Valid
          (Niagara|SetNiagaraVariable(Vector3) (Variables|Default|GetNS_IslandSpirit) "PivotLocation" (Variables|/Script/Engine.SceneComponent|GetRelativeLocation (Variables|Default|GetSpiritMesh)))
          (Niagara|SetNiagaraVariable(Float) (Variables|Default|GetNS_IslandSpirit) "Progress" _move))))
    (:Finished
      (Networking|SwitchHasAuthority
        (:Authority
          (CallFunction|AuthPossessNormal))))))

(event Custom|Server_StartSpawnEstrayPhantom
  (params (YawRotation :type Float%20%28double-precision%29))
  (bind _spline_spirit (Variables|Default|GetSpline_Spirit))
  (Transformation|SetActorRotation (Math|Rotator|MakeRotator 0.0 0.0 YawRotation))
  (bind _returnvalue (Game|SpawnActorfromClass "/Game/Blueprints/PF_Phantom.PF_Phantom_C" (Math|Transform|MakeTransform (Spline|GetLocationatSplinePoint _spline_spirit (- (Spline|GetNumberOfSplinePoints _spline_spirit) 1) "World") "0, 0, 0" "1.000000,1.000000,1.000000") "AlwaysSpawn" "MultiplyWithRoot" (Variables|Default|GetBP_PCS) 0 (Variables|Default|GetPSS) true 0 0))
  (bind _output_get (Variables|Default|SetSpawned_PF_Spirit _returnvalue))
  (Class|PlayerPhantom|MulticastSetLookRotation _output_get (Math|Rotator|MakeRotator 0.0 0.0 YawRotation))
  (Game|Player|SetViewTargetwithBlend (Variables|Default|GetBP_PCS) _output_get 1.5 "VTBlend_EaseInOut" 2.0 false)
  (CallFunction|MulticastStartSpawnDeadSpirit YawRotation))

(event Input|EnhancedActionEvents|EnhancedInputActionCameraRotate
  (params (ActionValue :type Vector%202D%20Structure) (ElapsedSeconds :type Float%20%28double-precision%29) (TriggeredSeconds :type Float%20%28double-precision%29) (InputAction :type Input%20Action%20Object%20Reference :default "/Game/Misc/EnhancedInput/CameraRotate.CameraRotate"))
  (bind (_x _y) (Math|Vector2D|BreakVector2D ActionValue))
  (bind _bp_gss (Variables|Default|GetBP_GSS))
  (bind _bp_gis (Variables|/Game/Blueprints/BP_GSS.BP_GSS_C|GetBP_GIS _bp_gss))
  (bind _localsettings (Variables|/Script/SkyCraft.GIS|GetLocalSettings _bp_gis))
  (bind _camerasensitivity (Variables|/Script/SkyCraft.LocalSettings|GetCameraSensitivity _localsettings))
  (Variables|Default|SetLookRotation (Math|Rotator|MakeRotator (.roll (Variables|Default|GetLookRotation)) (Math|Float|ClampAngle (+ (* _y _camerasensitivity (select (Variables|/Script/SkyCraft.LocalSettings|GetbInvertVerticalMouse _localsettings) -1.0 1.0)) (.pitch (Variables|Default|GetLookRotation))) -85.0 (Math|Float|SelectFloat 0.0 85.0 (Variables|/Script/SkyCraft.PlayerIsland|GetbIsCrystal (Variables|/Game/Blueprints/BP_PSS.BP_PSS_C|GetBP_PlayerIsland (Variables|Default|GetBP_PSS))))) (Math|Rotator|NormalizeAxis (+ (* _x _camerasensitivity) (.yaw (Variables|Default|GetLookRotation)))))))

(event Input|EnhancedActionEvents|EnhancedInputActionInventory
  (params (ActionValue :type Boolean) (ElapsedSeconds :type Float%20%28double-precision%29) (TriggeredSeconds :type Float%20%28double-precision%29) (InputAction :type Input%20Action%20Object%20Reference :default "/Game/Misc/EnhancedInput/Inventory.Inventory"))
  (Utilities|IsValid (Variables|Default|GetWidgetInventory)
    (:Is%20Valid
      _)
    (:Is%20Not%20Valid
      (bind _returnvalue (UserInterface|CreateWidget "/Game/Widgets/CWS/CWS_PF_Island_Inventory.CWS_PF_Island_Inventory_C"))
      (Variables|Default|SetWidgetInventory _returnvalue)))
  (UserInterface|Viewport|AddtoViewport (Variables|Default|GetWidgetInventory) 25)
  (Default|AddCWS (Variables|Default|GetBP_PSS) (Variables|Default|GetWidgetInventory) true true true "NewEnumerator2"))

(event Input|EnhancedActionEvents|EnhancedInputActionJump
  (params (ActionValue :type Boolean) (ElapsedSeconds :type Float%20%28double-precision%29) (TriggeredSeconds :type Float%20%28double-precision%29) (InputAction :type Input%20Action%20Object%20Reference :default "/Game/Misc/EnhancedInput/Jump.Jump"))
  (bind _returnvalue (Transformation|GetActorLocation))
  (bind _w_pf_island (Variables|Default|GetW_PF_Island))
  (bind _skyspringarmcomponent (Variables|Default|GetSkySpringArmComponent))
  (bind _w_pf_island_2 (Variables|Default|GetW_PF_Island))
  (bind _returnvalue_2 (Transformation|GetWorldRotation _skyspringarmcomponent))
  (bind _returnvalue_3 (+ _returnvalue "0, 0,100.000000"))
  (bind _circlprogressbar (Variables|/Game/Widgets/W_PF_Crystal.W_PF_Crystal_C|GetCirclProgressBar _w_pf_island_2))
  (bind _revivehint (Variables|/Game/Widgets/W_PF_Crystal.W_PF_Crystal_C|GetReviveHint _w_pf_island_2))
  (bind _circlprogressbar_2 (Variables|/Game/Widgets/W_PF_Crystal.W_PF_Crystal_C|GetCirclProgressBar _w_pf_island))
  (bind _returnvalue_4 (Math|Vector|GetForwardVector (Math|Rotator|MakeRotator 0.0 0.0 (.yaw _returnvalue_2))))
  (bind _returnvalue_5 (* _returnvalue_4 2e+02))
  (bind _returnvalue_6 (+ _returnvalue_5 _returnvalue_3))
  (:Started
    (Utilities|Hold/Tap 0.15 :!label _label
      (:HoldStart
        (Default|StartProgressBar _circlprogressbar)
        (Widget|SetVisibility _revivehint "Collapsed")
        (bind _progressvalue (Timeline|TimelineEmerge PlayFromStart)
          (:Update
            (Default|UpdateProgressBar _circlprogressbar_2 _progressvalue))
          (:Finished
            (Default|EndProgressBar _circlprogressbar_2)
            (if (Variables|/Script/SkyCraft.PlayerIsland|GetbIsCrystal (Variables|/Game/Blueprints/BP_PSS.BP_PSS_C|GetBP_PlayerIsland (Variables|Default|GetBP_PSS)))
              (bind (_outhit _returnvalue_7) (Collision|LineTraceByChannel _returnvalue_6 (+ _returnvalue_6 "0, 0,-400.000000") "TraceTypeQuery1" false 0 "None"))
              (if _returnvalue_7
                (CallFunction|ServerSpawnNormal (Math|Vector|MakeVectorNetQuantize (.x (.Location (Collision|BreakHitResult _outhit))) (.y (.Location (Collision|BreakHitResult _outhit))) (+ (.z (.Location (Collision|BreakHitResult _outhit))) 1e+02)) (.yaw (Transformation|GetWorldRotation (Variables|Default|GetSkySpringArmComponent))))
                (Input|DisableInput self (Variables|Default|GetBP_PCS)))
              (else
                (CallFunction|ServerStartSpawnEstrayPhantom (.yaw (Transformation|GetWorldRotation (Variables|Default|GetSkySpringArmComponent)))))))))
      (:HoldStop
        (Default|EndProgressBar _circlprogressbar)
        (Widget|SetVisibility _revivehint "SelfHitTestInvisible")
        (Timeline|TimelineEmerge Stop))))
  (:Completed
    (goto _label Released)))

(event EventEndPlay
  (params (EndPlayReason :type EEndPlayReason%20Enum :default "Destroyed"))
  (bind _ns_islandspirit (Variables|Default|GetNS_IslandSpirit))
  (Utilities|IsValid _ns_islandspirit
    (:Is%20Valid
      (Transformation|AttachComponentToComponent _ns_islandspirit (Variables|/Script/Engine.Actor|GetRootComponent (Actor|GetAttachParentActor)) "None" "KeepWorld" "KeepWorld" "KeepWorld" true)
      (Components|Activation|Deactivate (Variables|Default|GetNS_IslandSpirit)))))

(event Custom|CloseEyesAstralCompleted
  (bind _bp_pcs (Variables|Default|GetBP_PCS))
  (bind _returnvalue (UserInterface|CreateWidget "/Game/Widgets/W_BlackScreen.W_BlackScreen_C"))
  (bind _output_get (Variables|Default|SetAstralBlackScreen _returnvalue))
  (UserInterface|Viewport|AddtoViewport _output_get 100000)
  (Default|RemoveEyesTransition (Variables|Default|GetBP_PCS))
  (Rendering|SetVisibility (Variables|/Game/UltraDynamicSky/Blueprints/Ultra_Dynamic_Sky.Ultra_Dynamic_Sky_C|GetRoot (Variables|/Game/Blueprints/BP_PCS.BP_PCS_C|GetUDS (Variables|Default|GetBP_PCS))) false true)
  (Rendering|SetVisibility (Variables|/Script/Engine.SkyLight|GetLightComponent (Variables|/Game/Blueprints/BP_PCS.BP_PCS_C|GetAstral_SkyLight (Variables|Default|GetBP_PCS))) true false)
  (Default|ResetFOVEffect _bp_pcs (Pawn|GetControlledPawn _bp_pcs))
  (CallFunction|ServerReadyEnterAstral))

(event Custom|Client_ReadyEnterAstral
  (bind _bp_pcs (Variables|Default|GetBP_PCS))
  (Default|CreateEyesTransition _bp_pcs (delegate Custom|CloseEyesAstralCompleted) _bp_pcs false false))

(event Custom|Server_ReadyEnterAstral
  (bind _returnvalue (Math|Random|RandomFloatinRange -1e+02 -5e+01))
  (bind _returnvalue_2 (Math|Random|RandomBool))
  (bind _returnvalue_3 (Math|Random|RandomFloatinRange 5e+01 1e+02))
  (bind _bp_pcs (Variables|Default|GetBP_PCS))
  (bind _returnvalue_4 (Math|Float|SelectFloat _returnvalue_3 _returnvalue _returnvalue_2))
  (bind _astral (Default|Find/CreateAstral (Variables|Default|GetBP_GMS) (Variables|/Script/SkyCraft.PSS|GetPlayerIsland (Variables|Default|GetPSS))))
  (bind _returnvalue_5 (Game|SpawnActorfromClass "/Game/Blueprints/CharAstral.CharAstral_C" (Math|Transform|MakeTransform (Math|Vector|MakeVector (+ (.x (Transformation|GetActorLocation _astral)) _returnvalue_4) _returnvalue_4 100000304.0) "0, 0, 0" "1.000000,1.000000,1.000000") "AdjustIfPossibleButAlwaysSpawn" "MultiplyWithRoot" _bp_pcs _bp_pcs (Variables|Default|GetBP_PSS) _astral self (Variables|/Script/SkyCraft.InventoryComponent|GetSlots (Variables|Default|GetEquipmentInventoryComponent)) 0))
  (Pawn|Possess (Variables|Default|GetBP_PCS) _returnvalue_5)
  (CallFunction|ClientFinishEnterAstral))

(event Custom|Client_FinishEnterAstral
  (Default|HideBlack (Variables|Default|GetAstralBlackScreen) (delegate Custom|HideBlackCompleted_Event0)))

(event Custom|HideBlackCompleted_Event0
  (Widget|RemovefromParent (Variables|Default|GetAstralBlackScreen)))

(fn ConstructionScript)

(fn SpawnNormal
  (params (SpawnLocation :type Vector%20Net%20Quantize%20Structure) (YawRotation :type Float%20%28single-precision%29))
  (bind _returnvalue (Class|GMS|SpawnPlayerNormal (Variables|Default|GetBP_GMS) SpawnLocation (Math|Rotator|MakeRotator 0.0 0.0 YawRotation) (Variables|Default|GetBP_PCS) (Variables|Default|GetBP_PSS) (Variables|/Script/SkyCraft.InventoryComponent|GetSlots (Variables|Default|GetInventoryComponent)) (Variables|/Script/SkyCraft.InventoryComponent|GetSlots (Variables|Default|GetEquipmentInventoryComponent))))
  (bind _aspf_normal (Utilities|Casting|CastToPF_Normal _returnvalue))
  (Variables|Default|SetSpawned_PF_Normal _aspf_normal)
  (if (> (Variables|Default|GetPreservedHunger) -1.0)
    (Variables|/Script/SkyCraft.HungerComponent|SetHunger (Variables|/Script/SkyCraft.PlayerNormal|GetHungerComponent (Variables|Default|GetSpawned_PF_Normal)) (Variables|Default|GetPreservedHunger)))
  (Class|PlayerNormal|MulticastSetLookRotation (Variables|Default|GetSpawned_PF_Normal) (Math|Rotator|MakeRotator 0.0 0.0 YawRotation))
  (Variables|Default|SetEmerging true)
  (Game|Player|SetViewTargetwithBlend (Variables|Default|GetBP_PCS) (Variables|Default|GetSpawned_PF_Normal) 1.5 "VTBlend_EaseInOut" 2.0 false)
  (Default|OLDMulticastSetAttachedtoIA (Variables|Default|GetSpawned_PF_Normal) (Variables|/Game/Blueprints/BP_PSS.BP_PSS_C|GetBP_PlayerIsland (Variables|Default|GetBP_PSS)))
  (CallFunction|MulticastStartSpawnNormal YawRotation))

(fn AuthPossessNormal
  (bind _spawned_pf_normal (Variables|Default|GetSpawned_PF_Normal))
  (Rendering|SetActorHiddenInGame _spawned_pf_normal false)
  (Default|MulticastFXAppear _spawned_pf_normal)
  (Transformation|DetachFromActor (Variables|Default|GetSpawned_PF_Normal) "KeepWorld" "KeepWorld" "KeepWorld")
  (Pawn|Possess (Variables|Default|GetBP_PCS) (Variables|Default|GetSpawned_PF_Normal))
  (Actor|DestroyActor))

(fn GetLookRotation
  (return (Variables|Default|GetLookRotation)))

(fn SetLookRotation
  (params (LookRotation :type Rotator :default "0, 0, 0"))
  (bind _output_get (Variables|Default|SetLookRotation LookRotation))
  (return _output_get))