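; Actor component that streams BP_ChunkIsland chunks around its owner, with ticking enabled on the server.
; When the owner's grid coordinates change, it releases out-of-range chunks and fills a circular range, refreshing LOD on those kept.
; Chunks are shared through the BP_GMS registry via generator registration; new ones get coordinate-and-world-seed randomness and may spawn an IslandStatic, restoring saved data.
; It also reports island counts to clients and can inherit another Chunker's chunks.
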(event Custom|ForceBeginPlay
  (if (not (Variables|Default|GethadBeginPlay))
    (Variables|Default|SethadBeginPlay true)
    (if (Networking|IsServer)
      (bind _asbp_sgi (Utilities|Casting|CastToBP_SGI (Game|GetGameInstance))
        (:then
          _)
        (:CastFailed
          _))
      (Variables|Default|SetBP_SGI _asbp_sgi)
      (bind _asbp_gms (Utilities|Casting|CastToBP_GMS (Game|GetGameMode))
        (:then
          _)
        (:CastFailed
          _))
      (Variables|Default|SetBP_GMS _asbp_gms)
      (Utilities|Debug (Variables|/Game/Blueprints/BP_SGI.BP_SGI_C|GetDebugGlobal (Variables|Default|GetBP_SGI))
        (:Debug
          (if (Variables|/Game/Blueprints/BP_SGI.BP_SGI_C|GetisTestChunkIslandRenderRange (Variables|Default|GetBP_SGI))
            (Variables|/Game/Blueprints/BP_GMS.BP_GMS_C|SetChunkRenderRange (Variables|Default|GetBP_GMS) (Variables|/Game/Blueprints/BP_SGI.BP_SGI_C|GetTestChunkIslandRenderRange (Variables|Default|GetBP_SGI)))))
        (:Build
          _))
      (Components|Tick|SetComponentTickEnabled true))))

(event Custom|Server_ReturnIslands
  (bind _islands (CallFunction|ReturnIslands))
  (CallFunction|ClientReturnIslands _islands))

(event Custom|Client_ReturnIslands
  (params (Islands :type Integer))
  (Default|CallIslandStaticExpect (Variables|Default|GetBP_SGI) Islands))

(event EventEndPlay
  (params (EndPlayReason :type EEndPlayReason%20Enum :default "Destroyed"))
  (if (Networking|IsServer)
    (for _array_element (Variables|Default|GetRenderingChunks)
      (Default|RemoveGenerator _array_element self))))

(event EventTick
  (params (DeltaSeconds :type Float%20%28single-precision%29))
  (bind _output_get (Variables|Default|SetTickCoords (CallFunction|GetCoords)))
  (if (not (and (== (.x _output_get) (.x (Variables|Default|GetPreviousCoords))) (== (.y _output_get) (.y (Variables|Default|GetPreviousCoords))))) ; Player has changed Chunk Coordinates
    (Variables|Default|SetPreviousCoords (Variables|Default|GetTickCoords))
    (CallFunction|DestroyChunks)
    (CallFunction|SpawnChunks)))

(event EventBeginPlay
  (if (not (Variables|Default|GethadBeginPlay))
    (Variables|Default|SethadBeginPlay true)
    (if (Networking|IsServer)
      (bind _asbp_sgi (Utilities|Casting|CastToBP_SGI (Game|GetGameInstance))
        (:then
          _)
        (:CastFailed
          _))
      (Variables|Default|SetBP_SGI _asbp_sgi)
      (bind _asbp_gms (Utilities|Casting|CastToBP_GMS (Game|GetGameMode))
        (:then
          _)
        (:CastFailed
          _))
      (Variables|Default|SetBP_GMS _asbp_gms)
      (Utilities|Debug (Variables|/Game/Blueprints/BP_SGI.BP_SGI_C|GetDebugGlobal (Variables|Default|GetBP_SGI))
        (:Debug
          (if (Variables|/Game/Blueprints/BP_SGI.BP_SGI_C|GetisTestChunkIslandRenderRange (Variables|Default|GetBP_SGI))
            (Variables|/Game/Blueprints/BP_GMS.BP_GMS_C|SetChunkRenderRange (Variables|Default|GetBP_GMS) (Variables|/Game/Blueprints/BP_SGI.BP_SGI_C|GetTestChunkIslandRenderRange (Variables|Default|GetBP_SGI)))))
        (:Build
          _))
      (Components|Tick|SetComponentTickEnabled true))))

(fn GetCoords
  (bind _returnvalue (Components|GetOwner))
  (bind _bp_gms (Variables|Default|GetBP_GMS))
  (bind _returnvalue_2 (Transformation|GetActorLocation _returnvalue))
  (bind _chunksizexy (Variables|/Game/Blueprints/BP_GMS.BP_GMS_C|GetChunkSizeXY _bp_gms))
  (bind _returnvalue_3 (/ _returnvalue_2 _chunksizexy))
  (bind (_x _y) (Math|Vector|BreakVector _returnvalue_3))
  (return (Utilities|Struct|MakeInt2Vector (Math|Float|Round _x) (Math|Float|Round _y))))

(fn DestroyChunks
  (bind _bp_gms (Variables|Default|GetBP_GMS))
  (bind _bp_gms_2 (Variables|Default|GetBP_GMS))
  (bind _bp_gms_3 (Variables|Default|GetBP_GMS))
  (bind _chunksizexy (Variables|/Game/Blueprints/BP_GMS.BP_GMS_C|GetChunkSizeXY _bp_gms_2))
  (bind _chunksizexy_2 (Variables|/Game/Blueprints/BP_GMS.BP_GMS_C|GetChunkSizeXY _bp_gms_3))
  (LocalVariables|Set_CurrentCoords (CallFunction|GetCoords))
  (bind (_arrayindex _arrayelement) (Utilities|Array|ReverseforEachLoop (Variables|Default|GetRenderingCoords))
    (:LoopBody
      (LocalVariables|Set_Index _arrayindex)
      (if (>= (Math|Vector|Distance(Vector) (Math|Vector|MakeVector (* (.X (Utilities|Struct|BreakInt2Vector _arrayelement)) _chunksizexy) (* (.Y (Utilities|Struct|BreakInt2Vector _arrayelement)) _chunksizexy) 0.0) (Math|Vector|MakeVector (* (.x (LocalVariables|Get_CurrentCoords)) _chunksizexy_2) (* (.y (LocalVariables|Get_CurrentCoords)) _chunksizexy_2) 0.0)) (* (Variables|/Game/Blueprints/BP_GMS.BP_GMS_C|GetChunkRenderRange _bp_gms) (Variables|/Game/Blueprints/BP_GMS.BP_GMS_C|GetChunkSizeXY _bp_gms)))
        (Default|RemoveGenerator (Utilities|Array|Get(acopy) (Variables|Default|GetRenderingChunks) (LocalVariables|Get_Index)) self)
        (Utilities|Array|RemoveIndex (Variables|Default|GetRenderingCoords) (LocalVariables|Get_Index))
        (Utilities|Array|RemoveIndex (Variables|Default|GetRenderingChunks) (LocalVariables|Get_Index))))))

(fn SpawnChunks
  (bind _returnvalue (Class|KismetSystemLibrary|MakeLiteralInteger 200))
  (bind _returnvalue_2 (Class|KismetSystemLibrary|MakeLiteralInteger 50))
  (bind _bp_gms (Variables|Default|GetBP_GMS))
  (bind _bp_gms_2 (Variables|Default|GetBP_GMS))
  (bind _bp_gms_3 (Variables|Default|GetBP_GMS))
  (bind _bp_gms_4 (Variables|Default|GetBP_GMS))
  (bind _bp_gms_5 (Variables|Default|GetBP_GMS))
  (bind _bp_gms_6 (Variables|Default|GetBP_GMS))
  (bind _bp_gms_7 (Variables|Default|GetBP_GMS))
  (bind _chunksizexy (Variables|/Game/Blueprints/BP_GMS.BP_GMS_C|GetChunkSizeXY _bp_gms))
  (bind _chunksizexy_2 (Variables|/Game/Blueprints/BP_GMS.BP_GMS_C|GetChunkSizeXY _bp_gms_4))
  (bind _chunkrenderrange (Variables|/Game/Blueprints/BP_GMS.BP_GMS_C|GetChunkRenderRange _bp_gms_5))
  (bind _chunkrenderrange_2 (Variables|/Game/Blueprints/BP_GMS.BP_GMS_C|GetChunkRenderRange _bp_gms_7))
  (LocalVariables|Set_CurrentCoords (CallFunction|GetCoords))
  (for _index (range (* _chunkrenderrange -1) _chunkrenderrange)
    (LocalVariables|Set_LocalX _index)
    (for _index_2 (range (* _chunkrenderrange_2 -1) _chunkrenderrange_2)
      (LocalVariables|Set_LocalY _index_2)
      (LocalVariables|Set_ChunkWorldCoords (Utilities|Struct|MakeInt2Vector (+ (.x (LocalVariables|Get_CurrentCoords)) (LocalVariables|Get_LocalX)) (+ (.y (LocalVariables|Get_CurrentCoords)) (LocalVariables|Get_LocalY))))
      (if (< (Math|Vector|VectorLength (Math|Vector|MakeVector (* (LocalVariables|Get_LocalX) _chunksizexy) (* (LocalVariables|Get_LocalY) _chunksizexy) 0.0)) (* (Variables|/Game/Blueprints/BP_GMS.BP_GMS_C|GetChunkRenderRange _bp_gms_6) (Variables|/Game/Blueprints/BP_GMS.BP_GMS_C|GetChunkSizeXY _bp_gms_6)))
        (if (>= (Utilities|Array|FindItem (Variables|Default|GetRenderingCoords) (LocalVariables|Get_ChunkWorldCoords)) 0)
          (Default|UpdateLOD (Utilities|Array|Get(acopy) (Variables|Default|GetRenderingChunks) (Utilities|Array|FindItem (Variables|Default|GetRenderingCoords) (LocalVariables|Get_ChunkWorldCoords))))
          (elif (Utilities|Array|ContainsItem (Variables|/Game/Blueprints/BP_GMS.BP_GMS_C|GetSpawnedChunkIslandsCors (Variables|Default|GetBP_GMS)) (LocalVariables|Get_ChunkWorldCoords))
            (Utilities|Array|Add (Variables|Default|GetRenderingCoords) (LocalVariables|Get_ChunkWorldCoords))
            (Utilities|Array|Add (Variables|Default|GetRenderingChunks) (Utilities|Array|Get(acopy) (Variables|/Game/Blueprints/BP_GMS.BP_GMS_C|GetSpawnedChunkIslands _bp_gms_3) (Utilities|Array|FindItem (Variables|/Game/Blueprints/BP_GMS.BP_GMS_C|GetSpawnedChunkIslandsCors _bp_gms_3) (LocalVariables|Get_ChunkWorldCoords))))
            (Default|AddGenerator (Utilities|Array|Get(acopy) (Variables|/Game/Blueprints/BP_GMS.BP_GMS_C|GetSpawnedChunkIslands _bp_gms_3) (Utilities|Array|FindItem (Variables|/Game/Blueprints/BP_GMS.BP_GMS_C|GetSpawnedChunkIslandsCors _bp_gms_3) (LocalVariables|Get_ChunkWorldCoords))) self)
            (else
              (bind _returnvalue_3 (Game|SpawnActorfromClass "/Game/Blueprints/BP_ChunkIsland.BP_ChunkIsland_C" (Math|Transform|MakeTransform (Math|Vector|MakeVector (* (.x (LocalVariables|Get_ChunkWorldCoords)) _chunksizexy_2) (* (.y (LocalVariables|Get_ChunkWorldCoords)) _chunksizexy_2) 5e+04) "0, 0, 0" "1.000000,1.000000,1.000000") "AlwaysSpawn" "OverrideRootScale" 0 (Variables|Default|GetBP_GMS) (LocalVariables|Get_ChunkWorldCoords) (CallFunction|Int->Stream->Int (+ (CallFunction|Int->Stream->Int (.x (LocalVariables|Get_ChunkWorldCoords))) (.y (LocalVariables|Get_ChunkWorldCoords)) (Variables|/Game/Blueprints/BP_GMS.BP_GMS_C|GetWorldSeed (Variables|Default|GetBP_GMS)))) (Math|Random|RandomIntegerinRangefromStream (Math|Random|MakeRandomStream (CallFunction|Int->Stream->Int (+ (CallFunction|Int->Stream->Int (.x (LocalVariables|Get_ChunkWorldCoords))) (.y (LocalVariables|Get_ChunkWorldCoords)) (Variables|/Game/Blueprints/BP_GMS.BP_GMS_C|GetWorldSeed (Variables|Default|GetBP_GMS))))) _returnvalue_2 _returnvalue) (Math|Float|MapRangeClamped (Math|Conversions|ToFloat(Integer) (Math|Random|RandomIntegerinRangefromStream (Math|Random|MakeRandomStream (CallFunction|Int->Stream->Int (+ (CallFunction|Int->Stream->Int (.x (LocalVariables|Get_ChunkWorldCoords))) (.y (LocalVariables|Get_ChunkWorldCoords)) (Variables|/Game/Blueprints/BP_GMS.BP_GMS_C|GetWorldSeed (Variables|Default|GetBP_GMS))))) _returnvalue_2 _returnvalue)) (Math|Conversions|ToFloat(Integer) _returnvalue_2) (Math|Conversions|ToFloat(Integer) _returnvalue) 0.0 1.0) (Utilities|Array|MakeArray self) 0))
              (LocalVariables|Set_SpawnedChunk _returnvalue_3)
              (Utilities|FlowControl|Sequence
                (:then_0
                  (Utilities|Array|Add (Variables|/Game/Blueprints/BP_GMS.BP_GMS_C|GetSpawnedChunkIslands _bp_gms_2) (LocalVariables|Get_SpawnedChunk))
                  (Utilities|Array|Add (Variables|/Game/Blueprints/BP_GMS.BP_GMS_C|GetSpawnedChunkIslandsCors _bp_gms_2) (LocalVariables|Get_ChunkWorldCoords))
                  (Utilities|Array|Add (Variables|Default|GetRenderingChunks) (LocalVariables|Get_SpawnedChunk))
                  (Utilities|Array|Add (Variables|Default|GetRenderingCoords) (LocalVariables|Get_ChunkWorldCoords)))
                (:then_1
                  (if (Class|KismetMathLibrary|RandomBoolwithWeightfromStream (Math|Random|MakeRandomStream (CallFunction|Int->Stream->Int (CallFunction|Int->Stream->Int (+ (CallFunction|Int->Stream->Int (.x (LocalVariables|Get_ChunkWorldCoords))) (.y (LocalVariables|Get_ChunkWorldCoords)) (Variables|/Game/Blueprints/BP_GMS.BP_GMS_C|GetWorldSeed (Variables|Default|GetBP_GMS)))))) (Variables|Default|GetIslandsProbabilityWeight))
                    (if (.ReturnValue (Utilities|Map|Find (Variables|/Game/Blueprints/BP_GMS.BP_GMS_C|GetSavedIslandStatics (Variables|Default|GetBP_GMS)) (LocalVariables|Get_ChunkWorldCoords)))
                      (bind _returnvalue_4 (Game|SpawnActorfromClass "/Game/Blueprints/IslandStatic.IslandStatic_C" (Math|Transform|MakeTransform (Math|Vector|MakeVector (.x (Transformation|GetActorLocation (LocalVariables|Get_SpawnedChunk))) (.y (Transformation|GetActorLocation (LocalVariables|Get_SpawnedChunk))) (+ (.z (Transformation|GetActorLocation (LocalVariables|Get_SpawnedChunk))) (Math|Random|RandomFloatinRangefromStream (Math|Random|MakeRandomStream (Variables|/Game/Blueprints/BP_ChunkIsland.BP_ChunkIsland_C|GetSeed (LocalVariables|Get_SpawnedChunk))) 4e+04 4.5e+04))) "0, 0, 0" "1.000000,1.000000,1.000000") "AlwaysSpawn" "MultiplyWithRoot" 0 (LocalVariables|Get_SpawnedChunk) (LocalVariables|Get_ChunkWorldCoords) true (.Value (Utilities|Map|Find (Variables|/Game/Blueprints/BP_GMS.BP_GMS_C|GetSavedIslandStatics (Variables|Default|GetBP_GMS)) (LocalVariables|Get_ChunkWorldCoords))) 0))
                      (Variables|/Game/Blueprints/BP_ChunkIsland.BP_ChunkIsland_C|SetIslandStatic (LocalVariables|Get_SpawnedChunk) _returnvalue_4)
                      (Variables|/Game/Blueprints/IslandStatic.IslandStatic_C|SetChunk _returnvalue_4 (LocalVariables|Get_SpawnedChunk))
                      (else
                        (bind _returnvalue_5 (Game|SpawnActorfromClass :Class "/Game/Blueprints/IslandStatic.IslandStatic_C" :SpawnTransform (Math|Transform|MakeTransform (Math|Vector|MakeVector (.x (Transformation|GetActorLocation (LocalVariables|Get_SpawnedChunk))) (.y (Transformation|GetActorLocation (LocalVariables|Get_SpawnedChunk))) (+ (.z (Transformation|GetActorLocation (LocalVariables|Get_SpawnedChunk))) (Math|Random|RandomFloatinRangefromStream (Math|Random|MakeRandomStream (Variables|/Game/Blueprints/BP_ChunkIsland.BP_ChunkIsland_C|GetSeed (LocalVariables|Get_SpawnedChunk))) 4e+04 4.5e+04))) "0, 0, 0" "1.000000,1.000000,1.000000") :CollisionHandlingOverride "AlwaysSpawn" :TransformScaleMethod "MultiplyWithRoot" :Chunk (LocalVariables|Get_SpawnedChunk) :ChunkCoords (LocalVariables|Get_ChunkWorldCoords) :Instigator 0))
                        (Variables|/Game/Blueprints/BP_ChunkIsland.BP_ChunkIsland_C|SetIslandStatic (LocalVariables|Get_SpawnedChunk) _returnvalue_5)
                        (Variables|/Game/Blueprints/IslandStatic.IslandStatic_C|SetChunk _returnvalue_5 (LocalVariables|Get_SpawnedChunk))))))))))))))

(fn ReturnIslands
  (for _array_element (Variables|Default|GetRenderingChunks)
    (Utilities|IsValid (Variables|/Game/Blueprints/BP_ChunkIsland.BP_ChunkIsland_C|GetIslandStatic _array_element)
      (:Is%20Valid
        (LocalVariables|Set_Islands (+ 1 (LocalVariables|Get_Islands))))))
  (return (LocalVariables|Get_Islands)))

(fn TransferChunks
  (params (FromGenerator :type Chunker%20Object%20Reference))
  (Variables|Default|SetRenderingChunks (Variables|Chunker_C|GetRenderingChunks FromGenerator))
  (Variables|Default|SetRenderingCoords (Variables|Chunker_C|GetRenderingCoords FromGenerator))
  (Variables|Default|SetPreviousCoords (Variables|Chunker_C|GetPreviousCoords FromGenerator))
  (return))