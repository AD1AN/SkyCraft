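; BP_HealthSystem is a health system Blueprint that applies incoming damage to a Health value.
; ApplyDamageBasic looks up a multiplier in the NegateDamage map by the causer's indexed global damage type, scales the base damage by it and truncates the result.
; Only a positive result reduces Health, and the function then reports the hit as applied and flags destruction when Health reaches zero or below.
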(fn ApplyDamageBasic
  (params (In :type Apply%20Damage%20in%20Structure))
  (bind _output_get (LocalVariables|Set_NegatedDamage (Math|Float|Truncate (* (.Value (Utilities|Map|Find (Variables|Default|GetNegateDamage) (Utilities|Array|Get(acopy) (Variables|/Script/SkyCraft.DA_DamageCauserInfo|GetDamageGlobalTypes (.damagecauserinfo In)) (.indexdamageglobaltype In)))) (.BaseDamage (Utilities|Struct|BreakApplyDamageIn In))))))
  (if (> _output_get 0)
    (bind _output_get_2 (Variables|Default|SetHealth (- (Variables|Default|GetHealth) (LocalVariables|Get_NegatedDamage))))
    (if (<= _output_get_2 0)
      (return (Utilities|Struct|MakeApplyDamageOut true true))
      (else
        (return (Utilities|Struct|MakeApplyDamageOut true false))))
    (else
      (return ""))))