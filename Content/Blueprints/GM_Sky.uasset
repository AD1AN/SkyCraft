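; Game mode for the sky world that registers joining players with the game instance and saves and cleans up leaving ones.
; On startup it loads or creates the world's SaveGame slot, covering sky/weather, buildings, the moving player island, dead bodies and dropped items, with players saved by ID.
; It also lends pooled NavMeshBoundsVolumes to actors by attaching and rescaling them, and spawns a realm actor per island at spaced, high-altitude locations.
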(event Custom|SendMessageToEveryone
  (params (Sender :type String) (Message :type String))
  (for _array_element (Variables|/Game/Blueprints/SGI.SGI_C|GetPlayers (Variables|Default|GetSGI))
    (Default|AddMessagetoChat _array_element Sender Message)))

(event Custom|CustomBeginPlay
  (Variables|Default|SethadBeginPlayer true)
  (bind _outactors (Actor|GetAllActorsOfClass "/Script/NavigationSystem.NavMeshBoundsVolume"))
  (bind _output_get (Variables|Default|SetUnused_NMBV _outactors))
  (Utilities|FlowControl|Sequence
    (:then_0
      (for _array_element _output_get
        (Development|SetHiddeninGame (Variables|/Script/Engine.Brush|GetBrushComponent _array_element) false false)))
    (:then_1
      (bind _sgi (Class|BPISGI|GetSGI(Message) (Game|GetGameInstance)))
      (bind _output_get_2 (Variables|Default|SetSGI _sgi))
      (Variables|/Game/Blueprints/SGI.SGI_C|SetGM_Sky _output_get_2 self)
      (bind _gs_sky (Class|BPIGameMS|GetGSSky(Message) (Game|GetGameState)))
      (Variables|Default|SetGS_Sky _gs_sky)
      (Utilities|FlowControl|Sequence
        (:then_0
          (bind _returnvalue (Actor|GetActorOfClass "/Game/Blueprints/PlayerIsland.PlayerIsland_C"))
          (Variables|Default|SetPlayerIsland _returnvalue))
        (:then_1
          (bind _returnvalue_2 (Actor|GetActorOfClass "/Game/UltraDynamicSky/Blueprints/Ultra_Dynamic_Sky.Ultra_Dynamic_Sky_C"))
          (Variables|Default|SetUDS _returnvalue_2))
        (:then_2
          (bind _output_get_3 (Variables|Default|SetWorldName (Variables|/Game/Blueprints/SGI.SGI_C|GetWorldName (Variables|Default|GetSGI))))
          (bind _returnvalue_3 (SaveGame|DoesSaveGameExist _output_get_3))
          (if _returnvalue_3
            (CallFunction|LoadGame)
            (else
              (bind _returnvalue_4 (SaveGame|CreateSaveGameObject "/Game/Blueprints/SSG_World.SSG_World_C"))
              (SaveGame|SaveGametoSlot _returnvalue_4 (Variables|Default|GetWorldName)))))))))

(event Custom|DisconnectAllClients
  (for _array_element (Variables|/Game/Blueprints/SGI.SGI_C|GetPlayers (Variables|Default|GetSGI))
    (Default|ClientDisconnect _array_element)))

(event Custom|PlayerIslandCollision
  (bind _playerisland (Variables|Default|GetPlayerIsland))
  (Default|ServerStopPlayerIsland (Variables|Default|GetPlayerIsland))
  (Variables|/Game/Blueprints/PlayerIsland.PlayerIsland_C|SetCurrentDirection _playerisland "0, 0, 0")
  (Transformation|SetActorLocation (Variables|/Game/Blueprints/PlayerIsland.PlayerIsland_C|GetPreviousLocation _playerisland) false false))

(event EventBeginPlay
  (if (not (Variables|Default|GethadBeginPlayer))
    (CallFunction|CustomBeginPlay)))

(event EventOnLogout
  (params (ExitingController :type Controller%20Object%20Reference))
  (Variables|Default|SetTestNameClient (- (Variables|Default|GetTestNameClient) 1))
  (bind _pc_sky (Class|BPIPCSky|GetPCSky(Message) ExitingController))
  (Utilities|Array|RemoveItem (Variables|/Game/Blueprints/SGI.SGI_C|GetPlayers (Variables|Default|GetSGI)) _pc_sky)
  (bind _returnvalue (SaveGame|DoesSaveGameExist (Variables|Default|GetWorldName)))
  (if _returnvalue
    (bind _returnvalue_2 (SaveGame|LoadGamefromSlot (Variables|Default|GetWorldName)))
    (bind _ssg_world (Class|BPISSG|GetSSGWorld(Message) _returnvalue_2))
    (CallFunction|SavePlayer _ssg_world _pc_sky))
  (if (not (Variables|Default|GetLastSave))
    (switch Utilities|FlowControl|Switch|SwitchonE_CurrentPlayerForm (Variables|/Game/Blueprints/PC_Sky.PC_Sky_C|GetCurrentPlayerForm _pc_sky)
      (:NewEnumerator0
        (Actor|DestroyActor (Variables|/Game/Blueprints/PC_Sky.PC_Sky_C|GetPF_Island _pc_sky)))
      (:NewEnumerator2
        (Utilities|IsValid (Variables|/Game/Blueprints/PF_Normal.PF_Normal_C|GetPF_Spirit (Variables|/Game/Blueprints/PC_Sky.PC_Sky_C|GetPF_Normal _pc_sky))
          (:Is%20Valid
            (Actor|DestroyActor (Variables|/Game/Blueprints/PF_Normal.PF_Normal_C|GetPF_Spirit (Variables|/Game/Blueprints/PC_Sky.PC_Sky_C|GetPF_Normal _pc_sky))))
          (:Is%20Not%20Valid
            _))
        (Actor|DestroyActor (Variables|/Game/Blueprints/PC_Sky.PC_Sky_C|GetPF_Normal _pc_sky)))
      (:NewEnumerator3
        (Actor|DestroyActor (Variables|/Game/Blueprints/PF_Normal.PF_Normal_C|GetPF_Spirit (Variables|/Game/Blueprints/PC_Sky.PC_Sky_C|GetPF_Normal _pc_sky)))
        (Actor|DestroyActor (Variables|/Game/Blueprints/PC_Sky.PC_Sky_C|GetPF_Normal _pc_sky)))
      (:NewEnumerator1
        (Actor|DestroyActor (Variables|/Game/Blueprints/PC_Sky.PC_Sky_C|GetPF_Dead _pc_sky))))))

(event EventPostLogin
  (params (NewPlayer :type Player%20Controller%20Object%20Reference)))

(event EventHandleStartingNewPlayer
  (params (NewPlayer :type Player%20Controller%20Object%20Reference))
  (if (Variables|Default|GethadBeginPlayer)
    _
    (else
      (CallFunction|CustomBeginPlay)))
  (bind _pc_sky (Class|BPIPCSky|GetPCSky(Message) NewPlayer))
  (Variables|/Game/Blueprints/PC_Sky.PC_Sky_C|SetPlayerIsland _pc_sky (Variables|Default|GetPlayerIsland))
  (Default|ClientStart _pc_sky (Variables|Default|GetPlayerIsland))
  (Utilities|Array|Add (Variables|/Game/Blueprints/SGI.SGI_C|GetPlayers (Variables|Default|GetSGI)) _pc_sky))

(fn ConstructionScript)

(fn SaveGame
  (params (LastExitSave? :type Boolean))
  (bind _playerisland (Variables|Default|GetPlayerIsland))
  (if (not (Variables|Default|GetLastSave))
    (bind _returnvalue (SaveGame|DoesSaveGameExist (Variables|Default|GetWorldName)))
    (if _returnvalue
      (bind _returnvalue_2 (SaveGame|LoadGamefromSlot (Variables|Default|GetWorldName)))
      (bind _ssg_world (Class|BPISSG|GetSSGWorld(Message) _returnvalue_2))
      (LocalVariables|Set_SSG_World _ssg_world)
      (else
        (bind _returnvalue_3 (SaveGame|CreateSaveGameObject "/Game/Blueprints/SSG_World.SSG_World_C"))
        (LocalVariables|Set_SSG_World _returnvalue_3)))
    (Variables|/Game/Blueprints/SSG_World.SSG_World_C|SetLastPlayed (LocalVariables|Get_SSG_World) (Math|DateTime|Now))
    (Utilities|FlowControl|Sequence
      (:then_0
        ;[1 1 1 1 125] Sky & Weather
        (bind _packaged_state (Default|CreateUDSandUDWStateforSaving (Variables|Default|GetUDS)))
        (Variables|/Game/Blueprints/SSG_World.SSG_World_C|SetSky&Weather (LocalVariables|Get_SSG_World) _packaged_state))
      (:then_1
        (Utilities|FlowControl|Sequence
          (:then_0
            ;[1 0.2892 0.1795 1 55] Building Actors
            (Utilities|Array|Clear (Variables|/Game/Blueprints/SSG_World.SSG_World_C|GetSSG_BuildingActor (LocalVariables|Get_SSG_World)))
            (bind _outactors (Actor|GetAllActorsOfClass "/Game/Blueprints/Building/BuildingActor.BuildingActor_C"))
            (for _array_element _outactors
              (if (== (Components|GetOwner _array_element) 0) ; Check if this build not in Preview
                (Utilities|Array|Add (Variables|/Game/Blueprints/SSG_World.SSG_World_C|GetSSG_BuildingActor (LocalVariables|Get_SSG_World)) (Utilities|Struct|MakeSW_BuildingActor (Utilities|GetClass _array_element) (not (== (Actor|GetAttachParentActor _array_element) 0)) (Math|Transform|SelectTransform (Transformation|GetRelativeTransform (Variables|/Game/Blueprints/Building/BuildingActor.BuildingActor_C|GetScene _array_element)) (Transformation|GetActorTransform _array_element) (not (== (Actor|GetAttachParentActor _array_element) 0))) (Variables|/Game/Blueprints/Building/BuildingActor.BuildingActor_C|GetCurrentHealth _array_element) (Variables|/Game/Blueprints/Building/BuildingActor.BuildingActor_C|GetMaxHealth _array_element))))))
          (:then_1
            (Utilities|FlowControl|Sequence
              (:then_0
                ;[0.5141 1 0.5219 1 55] Player Island
                (Variables|/Game/Blueprints/SSG_World.SSG_World_C|SetSSG_PlayerIsland (LocalVariables|Get_SSG_World) (Utilities|Struct|MakeSW_PlayerIsland (Transformation|GetActorTransform _playerisland) (Variables|/Game/Blueprints/PlayerIsland.PlayerIsland_C|GetTargetDirection _playerisland) (Variables|/Game/Blueprints/PlayerIsland.PlayerIsland_C|GetTargetAltitude _playerisland) (Variables|/Game/Blueprints/PlayerIsland.PlayerIsland_C|GetTargetSpeed _playerisland) (Variables|/Game/Blueprints/PlayerIsland.PlayerIsland_C|GetStopIsland _playerisland) (Variables|/Game/Blueprints/PlayerIsland.PlayerIsland_C|GetEssence _playerisland) (Variables|/Game/Blueprints/PlayerIsland.PlayerIsland_C|GetEssenceBurnSelect _playerisland))))
              (:then_1
                (Utilities|FlowControl|Sequence
                  (:then_0
                    ;[0.05432 0.3611 1 1 55] Players
                    (for _array_element_2 (Variables|/Game/Blueprints/SGI.SGI_C|GetPlayers (Variables|Default|GetSGI))
                      (bind _output_get (LocalVariables|Set_ElementPC_Sky _array_element_2))
                      (CallFunction|SavePlayer (LocalVariables|Get_SSG_World) _output_get)))
                  (:then_1
                    (Utilities|FlowControl|Sequence
                      (:then_0
                        ;[0.2926 0.3021 0.2832 1 55] Char Dead
                        (Utilities|Array|Clear (Variables|/Game/Blueprints/SSG_World.SSG_World_C|GetSSG_Char_Dead (LocalVariables|Get_SSG_World)))
                        (bind _outactors_2 (Actor|GetAllActorsOfClass "/Game/Blueprints/PF_Dead.PF_Dead_C"))
                        (for _array_element_3 _outactors_2
                          (Utilities|IsValid (Variables|/Game/Blueprints/PF_Dead.PF_Dead_C|GetPC_Sky _array_element_3)
                            (:Is%20Not%20Valid
                              (Utilities|Array|Add (Variables|/Game/Blueprints/SSG_World.SSG_World_C|GetSSG_Char_Dead (LocalVariables|Get_SSG_World)) (Utilities|Struct|MakeSW_PF_Dead (Transformation|GetActorLocation _array_element_3) (Variables|/Game/Blueprints/PF_Dead.PF_Dead_C|GetEssence _array_element_3) (Variables|/Game/Blueprints/Inventory.Inventory_C|GetInventorySlots (Variables|/Game/Blueprints/PF_Dead.PF_Dead_C|GetInventory _array_element_3)) (Variables|/Game/Blueprints/PF_Dead.PF_Dead_C|GetCurrentLifeSpan _array_element_3)))))))
                      (:then_1
                        (Utilities|FlowControl|Sequence
                          (:then_0
                            ;[0.6042 1 0.952 1 55] Item Drop
                            (Utilities|Array|Clear (Variables|/Game/Blueprints/SSG_World.SSG_World_C|GetSSG_ItemDrop (LocalVariables|Get_SSG_World)))
                            (bind _outactors_3 (Actor|GetAllActorsOfClass "/Game/Blueprints/ItemDrop.ItemDrop_C"))
                            (for _array_element_4 _outactors_3
                              (Utilities|Array|Add (Variables|/Game/Blueprints/SSG_World.SSG_World_C|GetSSG_ItemDrop (LocalVariables|Get_SSG_World)) (Utilities|Struct|MakeSW_ItemDrop (Transformation|GetActorLocation _array_element_4) (Utilities|IsValid (Actor|GetAttachParentActor _array_element_4)) (Physics|IsSimulatingPhysics (Variables|/Game/Blueprints/ItemDrop.ItemDrop_C|GetStaticMesh _array_element_4) "None") (Variables|/Game/Blueprints/Inventory.Inventory_C|GetInventorySlots (Variables|/Game/Blueprints/ItemDrop.ItemDrop_C|GetAC_Inventory _array_element_4)) (Actor|GetLifeSpan _array_element_4)))))
                          (:then_1
                            (Utilities|FlowControl|Sequence
                              (:then_0
                                ;[1 0.09423 0.994 1 40] End save
                                (SaveGame|SaveGametoSlot (LocalVariables|Get_SSG_World) (Variables|Default|GetWorldName))
                                (Variables|Default|SetLastSave LastExitSave?)))))))))))))))))

(fn LoadGame
  (bind _returnvalue (SaveGame|LoadGamefromSlot (Variables|Default|GetWorldName)))
  (bind _ssg_world (Class|BPISSG|GetSSGWorld(Message) _returnvalue))
  (bind _output_get (LocalVariables|Set_SSG_World _ssg_world))
  (Variables|Default|SetWorldSeed (Variables|/Game/Blueprints/SSG_World.SSG_World_C|GetWorldSeed _output_get))
  (Utilities|FlowControl|Sequence
    (:then_0
      (Default|ApplySavedUDSandUDWState (Variables|Default|GetUDS) (Variables|/Game/Blueprints/SSG_World.SSG_World_C|GetSky&Weather (LocalVariables|Get_SSG_World))))
    (:then_1
      (Utilities|FlowControl|Sequence
        (:then_0
          (for _array_element (Variables|/Game/Blueprints/SSG_World.SSG_World_C|GetSSG_BuildingActor (LocalVariables|Get_SSG_World))
            (bind _returnvalue_2 (Game|SpawnActorfromClass :Class (.BuildingClass (Utilities|Struct|BreakSW_BuildingActor _array_element)) :SpawnTransform (.Transform (Utilities|Struct|BreakSW_BuildingActor _array_element)) :CollisionHandlingOverride "AlwaysSpawn" :Instigator 0))
            (if (.AttachedToPI (Utilities|Struct|BreakSW_BuildingActor _array_element))
              (Transformation|AttachActorToActor _returnvalue_2 (Variables|Default|GetPlayerIsland) "None" "KeepRelative" "KeepRelative" "KeepRelative" true))
            (Variables|/Game/Blueprints/Building/BuildingActor.BuildingActor_C|SetCurrentHealth _returnvalue_2 (.CurrentHealth (Utilities|Struct|BreakSW_BuildingActor _array_element)))
            (Variables|/Game/Blueprints/Building/BuildingActor.BuildingActor_C|SetMaxHealth _returnvalue_2 (.MaxHealth (Utilities|Struct|BreakSW_BuildingActor _array_element)))))
        (:then_1
          (Utilities|FlowControl|Sequence
            (:then_0
              (Variables|Default|SetPlayerIslandLoadedFromSave true)
              (Transformation|SetActorTransform (Variables|Default|GetPlayerIsland) (.Transform (Utilities|Struct|BreakSW_PlayerIsland (Variables|/Game/Blueprints/SSG_World.SSG_World_C|GetSSG_PlayerIsland (LocalVariables|Get_SSG_World)))) false true)
              (|PlayerIslandSet (.TargetDirection (Utilities|Struct|BreakSW_PlayerIsland (Variables|/Game/Blueprints/SSG_World.SSG_World_C|GetSSG_PlayerIsland (LocalVariables|Get_SSG_World)))) (.TargetAltitude (Utilities|Struct|BreakSW_PlayerIsland (Variables|/Game/Blueprints/SSG_World.SSG_World_C|GetSSG_PlayerIsland (LocalVariables|Get_SSG_World)))) (.TargetSpeed (Utilities|Struct|BreakSW_PlayerIsland (Variables|/Game/Blueprints/SSG_World.SSG_World_C|GetSSG_PlayerIsland (LocalVariables|Get_SSG_World)))) (.StopIsland (Utilities|Struct|BreakSW_PlayerIsland (Variables|/Game/Blueprints/SSG_World.SSG_World_C|GetSSG_PlayerIsland (LocalVariables|Get_SSG_World)))) (.Essence (Utilities|Struct|BreakSW_PlayerIsland (Variables|/Game/Blueprints/SSG_World.SSG_World_C|GetSSG_PlayerIsland (LocalVariables|Get_SSG_World)))) (.EssenceBurnSelect (Utilities|Struct|BreakSW_PlayerIsland (Variables|/Game/Blueprints/SSG_World.SSG_World_C|GetSSG_PlayerIsland (LocalVariables|Get_SSG_World))))))
            (:then_1
              (Utilities|FlowControl|Sequence
                (:then_0
                  (for _array_element_2 (Variables|/Game/Blueprints/SSG_World.SSG_World_C|GetSSG_Char_Dead (LocalVariables|Get_SSG_World))
                    (bind _returnvalue_3 (Game|SpawnActorfromClass "/Game/Blueprints/PF_Dead.PF_Dead_C" (Math|Transform|MakeTransform (.Location (Utilities|Struct|BreakSW_PF_Dead _array_element_2)) "0, 0, 0" "1.000000,1.000000,1.000000") "AlwaysSpawn" 0 0 0 0))
                    (Variables|/Game/Blueprints/PF_Dead.PF_Dead_C|SetEssence _returnvalue_3 (.Essence (Utilities|Struct|BreakSW_PF_Dead _array_element_2)))
                    (Variables|/Game/Blueprints/Inventory.Inventory_C|SetInventorySlots (Variables|/Game/Blueprints/PF_Dead.PF_Dead_C|GetInventory _returnvalue_3) (.Inventory (Utilities|Struct|BreakSW_PF_Dead _array_element_2)))
                    (Variables|/Game/Blueprints/PF_Dead.PF_Dead_C|SetCurrentLifeSpan _returnvalue_3 (.CurrentLifeSpan (Utilities|Struct|BreakSW_PF_Dead _array_element_2)))))
                (:then_1
                  (Utilities|FlowControl|Sequence
                    (:then_0
                      (for _array_element_3 (Variables|/Game/Blueprints/SSG_World.SSG_World_C|GetSSG_ItemDrop (LocalVariables|Get_SSG_World))
                        (bind _returnvalue_4 (Game|SpawnActorfromClass "/Game/Blueprints/ItemDrop.ItemDrop_C" (Math|Transform|MakeTransform (.Location (Utilities|Struct|BreakSW_ItemDrop _array_element_3)) "0, 0, 0" "1.000000,1.000000,1.000000") "AlwaysSpawn" 0 0))
                        (if (.AttachedToPI (Utilities|Struct|BreakSW_ItemDrop _array_element_3))
                          (Transformation|AttachActorToActor _returnvalue_4 (Variables|Default|GetPlayerIsland) "None" "KeepWorld" "KeepWorld" "KeepWorld" true))
                        (Physics|SetSimulatePhysics (Variables|/Game/Blueprints/ItemDrop.ItemDrop_C|GetStaticMesh _returnvalue_4) (.SimulatePhysics (Utilities|Struct|BreakSW_ItemDrop _array_element_3)))
                        (if (not (.SimulatePhysics (Utilities|Struct|BreakSW_ItemDrop _array_element_3)))
                          (Default|StartIdle _returnvalue_4))
                        (Actor|SetLifeSpan _returnvalue_4 (.RemainLifeSpan (Utilities|Struct|BreakSW_ItemDrop _array_element_3)))
                        (Variables|/Game/Blueprints/Inventory.Inventory_C|SetInventorySlots (Variables|/Game/Blueprints/ItemDrop.ItemDrop_C|GetAC_Inventory _returnvalue_4) (.Inventory (Utilities|Struct|BreakSW_ItemDrop _array_element_3)))))))))))))))

(fn SavePlayer
  (params (_SSG :type SSG%20World%20Object%20Reference) (_ElementPC_Sky :type PC%20Sky%20Object%20Reference))
  (bind _pf_normal (Variables|/Game/Blueprints/PC_Sky.PC_Sky_C|GetPF_Normal _ElementPC_Sky))
  (bind _pf_normal_2 (Variables|/Game/Blueprints/PC_Sky.PC_Sky_C|GetPF_Normal _ElementPC_Sky))
  (bind _currentplayerform (Variables|/Game/Blueprints/PC_Sky.PC_Sky_C|GetCurrentPlayerForm _ElementPC_Sky))
  (bind _pf_normal_3 (Variables|/Game/Blueprints/PC_Sky.PC_Sky_C|GetPF_Normal _ElementPC_Sky))
  (bind _pf_island (Variables|/Game/Blueprints/PC_Sky.PC_Sky_C|GetPF_Island _ElementPC_Sky))
  (bind _pf_dead (Variables|/Game/Blueprints/PC_Sky.PC_Sky_C|GetPF_Dead _ElementPC_Sky))
  (bind _currentplayerform_2 (Variables|/Game/Blueprints/PC_Sky.PC_Sky_C|GetCurrentPlayerForm _ElementPC_Sky))
  (bind _pf_normal_4 (Variables|/Game/Blueprints/PC_Sky.PC_Sky_C|GetPF_Normal _ElementPC_Sky))
  (bind _returnvalue (Utilities|Select :Index _currentplayerform_2 :NewEnumerator0 _pf_island :NewEnumerator2 _pf_normal_3 :NewEnumerator3 _pf_normal_3 :NewEnumerator1 _pf_dead))
  (bind _attachedtopi (Variables|/Game/Blueprints/PF_Normal.PF_Normal_C|GetAttachedToPI _pf_normal))
  (bind _inventory_equipment (Variables|/Game/Blueprints/PF_Normal.PF_Normal_C|GetInventory_Equipment _pf_normal_2))
  (bind _pf_spirit (Variables|/Game/Blueprints/PF_Normal.PF_Normal_C|GetPF_Spirit _pf_normal_4))
  (bind _inventoryslots (Variables|/Game/Blueprints/Inventory.Inventory_C|GetInventorySlots _inventory_equipment))
  (if (not (Variables|Default|GetLastSave))
    (Utilities|Struct|SetmembersinSW_Player (LocalVariables|Get_SavingPlayer) (Transformation|GetActorTransform _returnvalue))
    (bind _lookrotation (Class|BPILookRotation|GetLookRotation(Message) _returnvalue))
    (bind _essence (Class|BPIEssence|GetEssence(Message) _returnvalue))
    (bind _ac_inventory (Class|BPIGeneral|GetInventory(Message) _returnvalue))
    (Utilities|IsValid (Variables|/Game/Blueprints/PC_Sky.PC_Sky_C|GetPF_Normal _ElementPC_Sky)
      (:Is%20Valid
        (Utilities|Struct|SetmembersinSW_Player (LocalVariables|Get_SavingPlayer) _attachedtopi (Math|Transform|SelectTransform (Math|Transform|MakeTransform (Math|Transform|InverseTransformLocation (Transformation|GetActorTransform (Variables|Default|GetPlayerIsland)) (Transformation|GetActorLocation _pf_normal)) (Transformation|GetActorRotation _pf_normal) "1.000000,1.000000,1.000000") (Transformation|GetActorTransform _pf_normal) _attachedtopi) (Utilities|IsValid (Variables|/Game/Blueprints/PF_Normal.PF_Normal_C|GetPF_Spirit _pf_normal)))
        (Utilities|IsValid _pf_spirit
          (:Is%20Valid
            (Utilities|Struct|SetmembersinSW_Player (LocalVariables|Get_SavingPlayer) (Transformation|GetActorLocation _pf_spirit) (Variables|/Game/Blueprints/PF_Spirit.PF_Spirit_C|GetLookRotation _pf_spirit)))
          (:Is%20Not%20Valid
            _)))
      (:Is%20Not%20Valid
        _))
    (Utilities|Struct|SetmembersinSW_Player (LocalVariables|Get_SavingPlayer) (Variables|/Game/Blueprints/PC_Sky.PC_Sky_C|GetPlayerID _ElementPC_Sky) (Variables|/Game/Blueprints/PC_Sky.PC_Sky_C|GetCurrentPlayerForm _ElementPC_Sky) _lookrotation _essence (Utilities|Select :Index _currentplayerform :NewEnumerator0 0 :NewEnumerator2 (Variables|/Game/Blueprints/PC_Sky.PC_Sky_C|GetActiveQSI _ElementPC_Sky) :NewEnumerator3 (Variables|/Game/Blueprints/PC_Sky.PC_Sky_C|GetPrevQSI _ElementPC_Sky) :NewEnumerator1 0) (Variables|/Game/Blueprints/Inventory.Inventory_C|GetInventorySlots _ac_inventory) (Utilities|Select :Index _currentplayerform :NewEnumerator0 (Variables|/Game/Blueprints/Inventory.Inventory_C|GetInventorySlots (Variables|/Game/Blueprints/PF_Island.PF_Island_C|GetInventory_Equipment (Variables|/Game/Blueprints/PC_Sky.PC_Sky_C|GetPF_Island _ElementPC_Sky))) :NewEnumerator2 _inventoryslots :NewEnumerator3 _inventoryslots :NewEnumerator1 0))
    (Utilities|FlowControl|Sequence
      (:then_0
        (for (_array_element _array_index) (Variables|/Game/Blueprints/SSG_World.SSG_World_C|GetSSG_Player _SSG)
          (if (Utilities|Enum|Equal(Enum) (Utilities|Struct|BreakSW_Player _array_element) (Variables|/Game/Blueprints/PC_Sky.PC_Sky_C|GetPlayerID _ElementPC_Sky))
            (LocalVariables|Set_SavingPlayerFound true)
            (Utilities|Array|SetArrayElem (Variables|/Game/Blueprints/SSG_World.SSG_World_C|GetSSG_Player _SSG) _array_index (LocalVariables|Get_SavingPlayer))))
        (if (not (LocalVariables|Get_SavingPlayerFound))
          (Utilities|Array|Add (Variables|/Game/Blueprints/SSG_World.SSG_World_C|GetSSG_Player _SSG) (LocalVariables|Get_SavingPlayer))))
      (:then_1
        (SaveGame|SaveGametoSlot _SSG (Variables|Default|GetWorldName))))))

(fn NMBVUse
  (params (ActorUse :type Actor%20Object%20Reference) (ScaleNMBV :type Vector :default "1000.000000,1000.000000,500.000000"))
  (bind _unused_nmbv (Variables|Default|GetUnused_NMBV))
  (Utilities|Array|RemoveIndex _unused_nmbv)
  (bind _output_get (LocalVariables|Set_nmbv (Utilities|Array|Get(acopy) _unused_nmbv)))
  (Transformation|AttachActorToActor _output_get ActorUse "None" "KeepRelative" "KeepRelative" "KeepRelative" true)
  (Transformation|SetWorldScale3D (Variables|/Script/Engine.Brush|GetBrushComponent (LocalVariables|Get_nmbv)) ScaleNMBV)
  (Class|NavigationSystemV1|OnNavigationBoundsUpdated (Class|NavigationSystemV1|GetNavigationSystem) (LocalVariables|Get_nmbv))
  (return (LocalVariables|Get_nmbv)))

(fn NMBVUnuse
  (params (NMBV :type Nav%20Mesh%20Bounds%20Volume%20Object%20Reference%20%28by%20ref%29))
  (Utilities|Array|Add (Variables|Default|GetUnused_NMBV) NMBV)
  (Transformation|DetachFromActor NMBV "KeepRelative" "KeepRelative" "KeepRelative")
  (Transformation|SetWorldScale3D (Variables|/Script/Engine.Brush|GetBrushComponent NMBV) "1.000000,1.000000,1.000000")
  (return))

(fn CreateRealm
  (params (Island :type Actor%20Object%20Reference))
  (bind _islands (Variables|IslandRealm|GetIslands))
  (bind _returnvalue (Utilities|Array|LastIndex _islands))
  (if (!= _returnvalue 0)
    (bind _index (Utilities|FlowControl|ForLoopwithBreak 0 _returnvalue)
      (:LoopBody
        (if (not (== (* _index 200000) (.x (Transformation|GetActorLocation (Utilities|Array|Get(acopy) (Variables|IslandRealm|GetIslands) _index)))))
          (bind _returnvalue_2 (Game|SpawnActorfromClass "/Game/Blueprints/A_IslandRealm.A_IslandRealm_C" (Math|Transform|MakeTransform (Math|Vector|MakeVector (* _index 200000) 0.0 1e+08) "0, 0, 0" "1.000000,1.000000,1.000000") "AlwaysSpawn" 0 0))
          (Utilities|Array|Add (Variables|IslandRealm|GetIslands) Island)
          (Utilities|Array|Add (Variables|IslandRealm|GetRealms) _returnvalue_2)
          (return _returnvalue_2)))
      (:Completed
        (bind _returnvalue_3 (Game|SpawnActorfromClass "/Game/Blueprints/A_IslandRealm.A_IslandRealm_C" (Math|Transform|MakeTransform (Math|Vector|MakeVector (* (Utilities|Array|Length _islands) 200000) 0.0 1e+08) "0, 0, 0" "1.000000,1.000000,1.000000") "AlwaysSpawn" 0 0 :!label _label))
        (Utilities|Array|Add (Variables|IslandRealm|GetIslands) Island)
        (Utilities|Array|Add (Variables|IslandRealm|GetRealms) _returnvalue_3)
        (return _returnvalue_3)))
    (else
      (goto _label))))

(fn Find/CreateRealm
  (params (Island :type Actor%20Object%20Reference))
  (for (_array_element _array_index) (Variables|IslandRealm|GetIslands)
    (if (== _array_element Island)
      (return (Utilities|Array|Get(acopy) (Variables|IslandRealm|GetRealms) _array_index))))
  (bind _realm (IslandRealm|CreateRealm Island))
  (return _realm))

(fn GetGMSky
  (return self))

(fn GetGSSky
  (return 0))