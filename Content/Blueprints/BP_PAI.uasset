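; BP_PAI is a per-player actor owned by BP_PCS that acts as the hub for client-server requests and local UI.
; Server RPCs relay inventory, interaction, analysis, chat and IslandArchon commands, while tracking the current player form pawn.
; A stack of CWS widgets drives Escape handling, input mode and cursor.
; Astral entry chains client-server handshakes through temp camera, pawn possession and eye-close blackout; numpad debug keys alter essence.
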(event Custom|Server_AnalyzeEntity
  (params (DA_AnalyzeEntity :type DA%20Analyze%20Entity%20Object%20Reference%20%28by%20ref%29))
  (Utilities|Array|AddUnique (Variables|Default|GetAnalyzedEntities) DA_AnalyzeEntity)
  (Class|PAI|OnRepAnalyzedEntities))

(event Custom|Multicast_SetIslandArchon
  (params (IslandArchon :type Island%20Archon%20Object%20Reference))
  (bind _bp_pcs (Variables|Default|GetBP_PCS))
  (bind _output_get (Variables|Default|SetIslandArchon IslandArchon))
  (Utilities|IsValid _bp_pcs
    (:Is%20Valid
      (Variables|/Game/Blueprints/BP_PCS.BP_PCS_C|SetIslandArchon _bp_pcs _output_get))))

(event Custom|Server_DestroyActor
  (params (ActorDestroy :type Actor%20Object%20Reference))
  (Actor|DestroyActor ActorDestroy))

(event Custom|Client_ReceiveSavedPlayers
  (params (Keys :type Array%20of%20Strings) (Values :type Array%20of%20SS%20Player%20Structures))
  (for (_array_element _array_index) Keys
    (Utilities|Map|Add (Variables|/Game/Blueprints/BP_SGI.BP_SGI_C|GetSavedPlayers (Variables|Default|GetBP_SGI)) _array_element (Utilities|Array|Get(acopy) Values _array_index))))

(event Custom|Server_ResizeIsland
  (params (NewSize :type Integer))
  (Default|StartResizeIsland (Variables|Default|GetIslandArchon) NewSize))

(event Custom|Client_InterruptActor_BP_Internal
  (params (InterruptActor :type Actor%20Object%20Reference) (InterruptedBy :type EInterruptedBy%20Enum :default "Player") (InteractKey :type EInteractKey%20Enum :default "Interact1") (Pawn :type Pawn%20Object%20Reference) (BP_PAI :type BP%20PAI%20Object%20Reference))
  (Default|CallOnClientInterrupted (Actor|GetComponentbyClass InterruptActor "/Script/SkyCraft.InteractSystem") InterruptedBy InteractKey Pawn)
  (Class|InteractBP|ClientInterruptBP(Message) InterruptActor InterruptedBy InteractKey Pawn BP_PAI))

(event Custom|Multicast_Init
  (if (not (Variables|Default|GetInitialized))
    (Variables|Default|SetInitialized true)
    (bind _asbp_sgi (Utilities|Casting|CastToBP_SGI (Game|GetGameInstance))
      (:then
        _)
      (:CastFailed
        _))
    (Variables|Default|SetBP_SGI _asbp_sgi)
    (bind _asbp_pcs (Utilities|Casting|CastToBP_PCS (Components|GetOwner))
      (:then
        _)
      (:CastFailed
        _))
    (Variables|Default|SetBP_PCS _asbp_pcs)
    (Utilities|IsOwner
      (:Server
        (bind _asbp_gms (Utilities|Casting|CastToBP_GMS (Game|GetGameMode)))
        (Variables|Default|SetBP_GMS _asbp_gms))
      (:OwningClient
        (Variables|/Game/Blueprints/BP_SGI.BP_SGI_C|SetBP_PAI (Variables|Default|GetBP_SGI) self)
        (Input|EnableInput (Variables|Default|GetBP_PCS))
        (bind _returnvalue (UserInterface|CreateWidget "/Game/Widgets/W_Warning.W_Warning_C" (Variables|Default|GetBP_PCS)))
        (bind _output_get (Variables|Default|SetW_Warning _returnvalue))
        (UserInterface|Viewport|AddtoViewport _output_get 10000)))))

(event Custom|EnsureInit
  (if (not (Variables|Default|GetInitialized))
    (Variables|Default|SetInitialized true)
    (bind _asbp_sgi (Utilities|Casting|CastToBP_SGI (Game|GetGameInstance))
      (:then
        _)
      (:CastFailed
        _))
    (Variables|Default|SetBP_SGI _asbp_sgi)
    (bind _asbp_pcs (Utilities|Casting|CastToBP_PCS (Components|GetOwner))
      (:then
        _)
      (:CastFailed
        _))
    (Variables|Default|SetBP_PCS _asbp_pcs)
    (Utilities|IsOwner
      (:Server
        (bind _asbp_gms (Utilities|Casting|CastToBP_GMS (Game|GetGameMode)))
        (Variables|Default|SetBP_GMS _asbp_gms))
      (:OwningClient
        (Variables|/Game/Blueprints/BP_SGI.BP_SGI_C|SetBP_PAI (Variables|Default|GetBP_SGI) self)
        (Input|EnableInput (Variables|Default|GetBP_PCS))
        (bind _returnvalue (UserInterface|CreateWidget "/Game/Widgets/W_Warning.W_Warning_C" (Variables|Default|GetBP_PCS)))
        (bind _output_get (Variables|Default|SetW_Warning _returnvalue))
        (UserInterface|Viewport|AddtoViewport _output_get 10000)))))

(event Custom|Server_Interact_BP
  (params (InteractActor :type Actor%20Object%20Reference) (InteractKey :type EInteractKey%20Enum :default "Interact1") (Pawn :type Pawn%20Object%20Reference))
  (Class|InteractBP|ServerInteractBP(Message) InteractActor InteractKey Pawn self))

(event Custom|Server_IA_GiveEssence
  (params (GiveEssence :type Essence%20Structure))
  (Variables|/Game/Blueprints/IslandArchon.IslandArchon_C|SetEssence (Variables|Default|GetIslandArchon) (CallFunction|AddEssence GiveEssence (Variables|/Game/Blueprints/IslandArchon.IslandArchon_C|GetEssence (Variables|Default|GetIslandArchon))))
  (Variables|/Game/Blueprints/PF_Normal.PF_Normal_C|SetEssence (Variables|PlayerForms|GetPF_Normal) (CallFunction|SubtractEssence (Variables|/Game/Blueprints/PF_Normal.PF_Normal_C|GetEssence (Variables|PlayerForms|GetPF_Normal)) GiveEssence)))

(event Custom|Server_ToggleStopIA
  (bind _islandarchon (Variables|Default|GetIslandArchon))
  (if (Variables|/Game/Blueprints/IslandArchon.IslandArchon_C|GetStopIsland (Variables|Default|GetIslandArchon))
    (Default|UnstopIA _islandarchon)
    (else
      (Default|StopIA _islandarchon))))

(event Custom|Server_InterruptActor_BP
  (params (InterruptActor :type Actor%20Object%20Reference) (InterruptedBy :type EInterruptedBy%20Enum :default "Player") (InteractKey :type EInteractKey%20Enum :default "Interact1") (Pawn :type Pawn%20Object%20Reference) (BP_PAI :type BP%20PAI%20Object%20Reference))
  (bind _returnvalue (Actor|GetComponentbyClass InterruptActor "/Script/SkyCraft.InteractSystem"))
  (Class|InteractSystem|RemoveProlonged _returnvalue Pawn)
  (Default|CallOnServerInterrupted _returnvalue InterruptedBy InteractKey Pawn)
  (Class|InteractBP|ServerInterruptBP(Message) InterruptActor InterruptedBy InteractKey Pawn BP_PAI)
  (CallFunction|ClientInterruptActorBPInternal InterruptActor InterruptedBy InteractKey Pawn BP_PAI))

(event Custom|Server_SendMessageEveryone
  (params (Sender :type String) (Message :type String))
  ;[1 1 1] Chat
  (Default|MessagePlayer (Variables|Default|GetBP_GMS) Sender Message))

(event Custom|Server_AnalyzeItem
  (params (DA_Item :type DA%20Item%20Object%20Reference%20%28by%20ref%29))
  (Utilities|Array|AddUnique (Variables|Default|GetAnalyzedItems) DA_Item)
  (Class|PAI|OnRepAnalyzedItems))

(event Custom|Client_Disconnect
  (if (not (Networking|IsDedicatedServer))
    (if (Pawn|IsLocalController (Variables|Default|GetBP_PCS))
      (|DestroySession (Variables|Default|GetBP_PCS)
        (:then
          (Game|OpenLevel(byObjectReference) "/Game/Levels/MainMenu.MainMenu"))))))

(event Custom|Server_SetEssence
  (params (Actor :type Actor%20Object%20Reference) (Essence :type Essence%20Structure))
  (Class|BPIEssence|SetEssence(Server)(Message) Actor Essence))

(event Custom|Server_AnalyzeIsland
  (params (IslandStatic :type Island%20Static%20Object%20Reference))
  (CallFunction|ClientAnalyzedIsland IslandStatic))

(event Custom|Client_AnalyzedIsland
  (params (IslandStatic :type Island%20Static%20Object%20Reference))
  (bind _pf_normal (Variables|PlayerForms|GetPF_Normal))
  (Variables|/Game/Blueprints/PF_Normal.PF_Normal_C|SetcanAnalyze _pf_normal true)
  (bind _returnvalue (UserInterface|CreateWidget "/Game/Widgets/CWS/CWS_AnalyzedIsland.CWS_AnalyzedIsland_C" 0 IslandStatic _pf_normal))
  (CallFunction|AddCWS _returnvalue true true "NewEnumerator2")
  (UserInterface|Viewport|AddtoViewport _returnvalue 15))

(event Custom|Server_Inventory_Swap
  (params (Inventory :type Inventory%20Object%20Reference) (SlotIndex :type Integer) (OtherInventory :type Inventory%20Object%20Reference) (OtherSlotIndex :type Integer))
  (Class|Inventory|Swap Inventory SlotIndex OtherInventory OtherSlotIndex))

(event Custom|Server_Inventory_InsertSlot
  (params (Inventory :type Inventory%20Object%20Reference) (InsertingSlot :type Slot%20Structure))
  (Class|Inventory|InsertSlot Inventory InsertingSlot))

(event Custom|Server_IA_SpeedChange
  (params (TargetSpeed :type Float%20%28double-precision%29) (IslandArchon :type Island%20Archon%20Object%20Reference))
  (Variables|/Game/Blueprints/IslandArchon.IslandArchon_C|SetTargetSpeed IslandArchon (Math|Float|Clamp(Float) TargetSpeed 1.0 1e+02)))

(event Custom|Client_ClearCWS
  (for _array_element (Variables|Default|GetStack_CWS)
    (CallFunction|RemoveCWS _array_element true true)))

(event Custom|Client_MessageWorld
  (params (Message :type String) (MessageWorld :type E_MessageWorld%20Enum :default "NewEnumerator0"))
  ;[1 1 1] Chat
  (Default|MessageWorld (Variables|Default|GetW_Chat) Message MessageWorld))

(event Custom|Server_MulticastClearCWS
  (Default|AllClientsClearCWS (Variables|Default|GetBP_SGI)))

(event Custom|Multicast_PlayerForm_Possessed
  (params (CurrentPlayerForm :type EPlayerForm%20Enum :default "Island") (PlayerForm_Possess :type Actor%20Object%20Reference))
  (bind _output_get (Variables|PlayerForms|SetCurrentPF CurrentPlayerForm))
  (bind (_pf_island _pf_normal _pf_spirit _pf_dead) (Class|BPIPlayerForm|GetPlayerForm(Message) PlayerForm_Possess))
  (switch Utilities|FlowControl|Switch|SwitchonEPlayerForm _output_get
    (:Island
      (Variables|PlayerForms|SetPF_Island _pf_island))
    (:Normal
      (Variables|PlayerForms|SetPF_Normal _pf_normal))
    (:Spirit
      (Variables|PlayerForms|SetPF_Spirit _pf_spirit))
    (:Dead
      (Variables|PlayerForms|SetPF_Dead _pf_dead))))

(event Custom|Server_Inventory_Spend
  (params (Inventory :type Inventory%20Object%20Reference) (SpendSlot :type Slot%20Structure))
  (Class|Inventory|Spend Inventory SpendSlot))

(event Custom|Server_AddProlonged
  (params (InteractSystem :type Interact%20System%20Object%20Reference) (InteractKey :type EInteractKey%20Enum :default "Interact1") (InteractedPawn :type Pawn%20Object%20Reference))
  (Class|InteractSystem|AddProlonged InteractSystem (Utilities|Struct|MakeCurrentProlonged InteractKey InteractedPawn self)))

(event Custom|Server_Interact_CPP
  (params (InteractActor :type Actor%20Object%20Reference) (InteractKey :type EInteractKey%20Enum :default "Interact1") (Pawn :type Pawn%20Object%20Reference))
  (Class|InteractCPP|ServerInteract(Message) InteractActor (Utilities|Struct|MakeInteractIn InteractKey Pawn self)))

(event Custom|Server_SetPawnIslandControl
  (params (Pawn :type Pawn%20Object%20Reference))
  (bind _islandarchon (Variables|Default|GetIslandArchon))
  (bind _pawn_island_control (Variables|/Game/Blueprints/IslandArchon.IslandArchon_C|GetPawn%20Island%20Control _islandarchon))
  (Default|MulticastPossessControlPawn _pawn_island_control Pawn self)
  (Game|Player|SetViewTargetwithBlend (Variables|Default|GetBP_PCS) _pawn_island_control 1.0 "VTBlend_EaseInOut" 2.0 false)
  (Default|PossessPawn (Variables|Default|GetBP_PCS) _pawn_island_control true))

(event Custom|Client_ReceiveMessageEveryone
  (params (Sender :type String) (Message :type String))
  ;[1 1 1] Chat
  (Default|ReceiveMessagePlayer (Variables|Default|GetW_Chat) Sender Message))

(event Custom|Server_Inventory_ChangeSlot
  (params (Inventory :type Inventory%20Object%20Reference) (SlotIndex :type Integer) (NewSlot :type Slot%20Structure))
  (Class|Inventory|MulticastChangeSlot Inventory SlotIndex NewSlot))

(event Custom|Server_Inventory_DropIn
  (params (Inventory :type Inventory%20Object%20Reference) (SlotIndex :type Integer) (DragInventory :type Inventory%20Object%20Reference) (DragSlotIndex :type Integer) (DragQuantity :type Byte))
  (Class|Inventory|Dropin Inventory SlotIndex DragInventory DragSlotIndex DragQuantity))

(event Input|EnhancedActionEvents|EnhancedInputActionChat
  (params (ActionValue :type Boolean) (ElapsedSeconds :type Float%20%28double-precision%29) (TriggeredSeconds :type Float%20%28double-precision%29) (InputAction :type Input%20Action%20Object%20Reference :default "/Game/Misc/EnhancedInput/Chat.Chat"))
  (bind _bp_pcs (Variables|Default|GetBP_PCS))
  ;[1 1 1] Chat
  (:Started
    (if (Class|PCS|IsPawnInputEnabled _bp_pcs (Pawn|GetControlledPawn _bp_pcs))
      (Default|FocusChat (Variables|Default|GetW_Chat)))))

(event Input|EnhancedActionEvents|EnhancedInputActionCursorMode
  (params (ActionValue :type Boolean) (ElapsedSeconds :type Float%20%28double-precision%29) (TriggeredSeconds :type Float%20%28double-precision%29) (InputAction :type Input%20Action%20Object%20Reference :default "/Game/Misc/EnhancedInput/CursorMode.CursorMode")))

(event EventBeginPlay
  (CallFunction|EnsureInit)
  (Utilities|IsOwner
    (:OwningClient
      (bind _returnvalue (UserInterface|CreateWidget "/Game/Widgets/W_Chat.W_Chat_C" (Variables|Default|GetBP_PCS) self))
      (bind _output_get (Variables|Default|SetW_Chat _returnvalue))
      (UserInterface|Viewport|AddtoViewport _output_get 10)
      (Default|ClientStartPlayer (Variables|Default|GetBP_PCS)))))

(event Input|KeyboardEvents|Escape
  (params (Key :type Key%20Structure :default "None"))
  (bind _stack_cws (Variables|Default|GetStack_CWS))
  (bind _bp_pcs (Variables|Default|GetBP_PCS))
  (bind _returnvalue (Utilities|Array|LastIndex _stack_cws))
  (bind _output (Utilities|Array|Get(acopy) _stack_cws _returnvalue))
  ;[1 1 1] Escape
  (:Pressed
    (if (Utilities|Array|IsEmpty (Variables|Default|GetStack_CWS)) ; If empty
      (bind _returnvalue_2 (UserInterface|CreateWidget "/Game/Widgets/CWS/CWS_EscapeMenu.CWS_EscapeMenu_C" _bp_pcs (Pawn|GetControlledPawn _bp_pcs)))
      (CallFunction|AddCWS _returnvalue_2 true true "NewEnumerator2")
      (UserInterface|Viewport|AddtoViewport _returnvalue_2 1000)
      (else
        (bind _canremove (Default|OnEscapeCWS _output))
        (if _canremove
          (CallFunction|RemoveCWS _output (Variables|/Game/Widgets/CWS/CWS.CWS_C|GetInitial_RemoveFromStack _output) (Variables|/Game/Widgets/CWS/CWS.CWS_C|GetInitial_RemoveFromParent _output)))))))

(event Custom|Client_LeaveAstral
  (Rendering|SetVisibility (Variables|/Game/UltraDynamicSky/Blueprints/Ultra_Dynamic_Sky.Ultra_Dynamic_Sky_C|GetRoot (Variables|/Game/Blueprints/BP_PCS.BP_PCS_C|GetUDS (Variables|Default|GetBP_PCS))) true true)
  (Rendering|SetVisibility (Variables|/Script/Engine.SkyLight|GetLightComponent (Variables|/Game/Blueprints/BP_PCS.BP_PCS_C|GetAstral_SkyLight (Variables|Default|GetBP_PCS))) false false))

(event Custom|CloseEyesAstralCompleted
  (bind _bp_pcs (Variables|Default|GetBP_PCS))
  (bind _returnvalue (UserInterface|CreateWidget "/Game/Widgets/W_BlackScreen.W_BlackScreen_C"))
  (bind _output_get (Variables|Default|SetLatestBlackScreen _returnvalue))
  (UserInterface|Viewport|AddtoViewport _output_get 100000)
  (Default|RemoveEyesTransition (Variables|Default|GetBP_PCS))
  (Rendering|SetVisibility (Variables|/Game/UltraDynamicSky/Blueprints/Ultra_Dynamic_Sky.Ultra_Dynamic_Sky_C|GetRoot (Variables|/Game/Blueprints/BP_PCS.BP_PCS_C|GetUDS (Variables|Default|GetBP_PCS))) false true)
  (Rendering|SetVisibility (Variables|/Script/Engine.SkyLight|GetLightComponent (Variables|/Game/Blueprints/BP_PCS.BP_PCS_C|GetAstral_SkyLight (Variables|Default|GetBP_PCS))) true false)
  (Default|ResetFOVEffect _bp_pcs (Pawn|GetControlledPawn _bp_pcs))
  (CallFunction|ServerReadyEnterAstral))

(event Custom|Server_LeaveAstral
  (params (CharAstral :type Char%20Astral%20Object%20Reference))
  (Default|PossessPawn (Variables|Default|GetBP_PCS) (Variables|PlayerForms|GetPF_Island) true)
  (CallFunction|ClientLeaveAstral)
  (Actor|DestroyActor CharAstral))

(event Custom|Client_ReadyEnterAstral
  (bind _bp_pcs (Variables|Default|GetBP_PCS))
  (Default|CreateEyesTransition _bp_pcs (delegate Custom|CloseEyesAstralCompleted) _bp_pcs false false))

(event Custom|Server_ReadyEnterAstral
  (bind _returnvalue (Math|Random|RandomFloatinRange -1e+02 -5e+01))
  (bind _returnvalue_2 (Math|Random|RandomBool))
  (bind _returnvalue_3 (Math|Random|RandomFloatinRange 5e+01 1e+02))
  (bind _bp_pcs (Variables|Default|GetBP_PCS))
  (bind _returnvalue_4 (Math|Float|SelectFloat _returnvalue_3 _returnvalue _returnvalue_2))
  (bind _astral (Default|Find/CreateAstral (Variables|Default|GetBP_GMS) (Variables|Default|GetIslandArchon)))
  (bind _returnvalue_5 (Game|SpawnActorfromClass "/Game/Blueprints/CharAstral.CharAstral_C" (Math|Transform|MakeTransform (Math|Vector|MakeVector (+ (.x (Transformation|GetActorLocation _astral)) _returnvalue_4) _returnvalue_4 100000304.0) "0, 0, 0" "1.000000,1.000000,1.000000") "AdjustIfPossibleButAlwaysSpawn" "MultiplyWithRoot" _bp_pcs _bp_pcs self _astral (Variables|/Game/Blueprints/BP_PCS.BP_PCS_C|GetCharacterBio _bp_pcs) 0))
  (Default|PossessPawn (Variables|Default|GetBP_PCS) _returnvalue_5 true)
  (CallFunction|ClientFinishEnterAstral))

(event Custom|Client_FinishEnterAstral
  (Default|HideBlack (Variables|Default|GetLatestBlackScreen) (delegate Custom|HideBlackCompleted_Event0)))

(event Custom|Server_EnterAstral
  (bind _pf_normal (Variables|PlayerForms|GetPF_Normal))
  (switch Utilities|FlowControl|Switch|SwitchonEPlayerForm (Variables|PlayerForms|GetCurrentPF)
    (:Island
      (CallFunction|ClientReadyEnterAstral))
    (:Normal
      (bind _returnvalue (Game|SpawnActorfromClass "/Game/Blueprints/PawnTempCamera.PawnTempCamera_C" (Math|Transform|MakeTransform (Transformation|GetWorldLocation (Variables|/Game/Blueprints/PF_Normal.PF_Normal_C|GetMainCamera _pf_normal)) (Variables|/Game/Blueprints/PF_Normal.PF_Normal_C|GetLookRotation _pf_normal) "1.000000,1.000000,1.000000") "AlwaysSpawn" "MultiplyWithRoot" (Variables|Default|GetBP_PCS) 3.0 true (Variables|Default|GetIslandArchon) 0))
      (EventDispatchers|BindEventtoClientInitialized _returnvalue (delegate Custom|ClientInitialized))
      (Default|ClientInitialize _returnvalue))))

(event Custom|HideBlackCompleted_Event0
  (Widget|RemovefromParent (Variables|Default|GetLatestBlackScreen)))

(event Custom|ClientInitialized
  (bind _bp_pcs (Variables|Default|GetBP_PCS))
  (bind _pf_normal (Variables|PlayerForms|GetPF_Normal))
  (bind _returnvalue (Game|SpawnActorfromClass "/Game/Blueprints/PF_Island.PF_Island_C" (Math|Transform|MakeTransform "0, 0, 0" "0, 0, 0" "1.000000,1.000000,1.000000") "AlwaysSpawn" "MultiplyWithRoot" _bp_pcs _bp_pcs self 0))
  (Default|MulticastSetLookRotation _returnvalue (Variables|/Game/Blueprints/PF_Normal.PF_Normal_C|GetLookRotation (Variables|PlayerForms|GetPF_Normal)))
  (Transformation|AttachActorToActor _returnvalue (Variables|Default|GetIslandArchon) "None" "KeepRelative" "KeepRelative" "KeepRelative" true)
  (Default|MulticastNormaltoIslandFX (Variables|PlayerForms|GetPF_Normal))
  (Default|MulticastInitSetup _returnvalue (Variables|/Game/Blueprints/PF_Normal.PF_Normal_C|GetEssence _pf_normal) (Variables|/Script/SkyCraft.Inventory|GetSlots (Variables|/Game/Blueprints/PF_Normal.PF_Normal_C|GetInventory _pf_normal)) (Variables|/Script/SkyCraft.Inventory|GetSlots (Variables|/Game/Blueprints/PF_Normal.PF_Normal_C|GetInventoryEquipment _pf_normal)))
  (Game|Player|SetViewTargetwithBlend (Variables|Default|GetBP_PCS) _returnvalue 1.0 "VTBlend_EaseInOut" 2.0 false)
  (Default|PossessPawn (Variables|Default|GetBP_PCS) _returnvalue true)
  (Default|ServerDestroyHandle (Variables|PlayerForms|GetPF_Normal))
  (CallFunction|ClientReadyEnterAstral))

(event Input|EnhancedActionEvents|EnhancedInputActionCinematicCamera
  (params (ActionValue :type Boolean) (ElapsedSeconds :type Float%20%28double-precision%29) (TriggeredSeconds :type Float%20%28double-precision%29) (InputAction :type Input%20Action%20Object%20Reference :default "/Game/Misc/EnhancedInput/CinematicCamera.CinematicCamera")))

(event Input|KeyboardEvents|NumPadOne
  (params (Key :type Key%20Structure :default "None"))
  (:Pressed
    (Class|BPIEssence|SetEssence(Server)(Message) (Pawn|GetControlledPawn (Variables|Default|GetBP_PCS)))))

(event Input|KeyboardEvents|NumPadSeven
  (params (Key :type Key%20Structure :default "None"))
  (:Pressed
    (Class|BPIEssence|ConsumeEssence(Message) (Pawn|GetControlledPawn (Variables|Default|GetBP_PCS)) (Utilities|Struct|MakeEssence 100000 0 0))))

(event Input|KeyboardEvents|NumPadEight
  (params (Key :type Key%20Structure :default "None"))
  (:Pressed
    (Class|BPIEssence|ConsumeEssence(Message) (Pawn|GetControlledPawn (Variables|Default|GetBP_PCS)) (Utilities|Struct|MakeEssence 0 100000 0))))

(event Input|KeyboardEvents|NumPadNine
  (params (Key :type Key%20Structure :default "None"))
  (:Pressed
    (Class|BPIEssence|ConsumeEssence(Message) (Pawn|GetControlledPawn (Variables|Default|GetBP_PCS)) (Utilities|Struct|MakeEssence 0 0 100000))))

(fn ConstructionScript)

(fn AddCWS
  (params (AddCWS :type CWS%20Object%20Reference) (DisablePawnInput :type Boolean) (ShowCursor :type Boolean) (InputMode :type E_InputMode%20Enum :default "NewEnumerator2"))
  (bind _bp_pcs (Variables|Default|GetBP_PCS))
  (LocalVariables|SetIndexPreviousCWS (Utilities|Array|LastIndex (Variables|Default|GetStack_CWS)))
  (Utilities|Array|Add (Variables|Default|GetStack_CWS) AddCWS)
  (if (> (LocalVariables|GetIndexPreviousCWS) -1) ; If already had CWS?
    (Class|BPIInputAction|UnbindInputActions(Message) (Utilities|Array|Get(acopy) (Variables|Default|GetStack_CWS) (LocalVariables|GetIndexPreviousCWS)))
    (Class|BPIInputAction|AssignInputActions(Message) AddCWS)
    (else
      (Utilities|FlowControl|Sequence
        (:then_0
          (if DisablePawnInput
            (Input|DisableInput (Pawn|GetControlledPawn _bp_pcs) _bp_pcs)))
        (:then_1
          (if ShowCursor
            (Variables|/Script/Engine.PlayerController|SetbShowMouseCursor (Variables|Default|GetBP_PCS) true)))
        (:then_2
          (Class|BPIInputAction|AssignInputActions(Message) AddCWS)
          (switch Utilities|FlowControl|Switch|SwitchonE_InputMode InputMode
            (:NewEnumerator0
              (Input|SetInputModeGameOnly (Variables|Default|GetBP_PCS) false))
            (:NewEnumerator1
              (Input|SetInputModeUIOnly (Variables|Default|GetBP_PCS) AddCWS "DoNotLock" false))
            (:NewEnumerator2
              (Input|SetInputModeGameandUI (Variables|Default|GetBP_PCS) AddCWS "DoNotLock" false false))))))))

(fn RemoveCWS
  (params (RemoveCWS :type CWS%20Object%20Reference) (RemoveFromStack :type Boolean) (RemoveFromParent :type Boolean))
  (bind _stack_cws (Variables|Default|GetStack_CWS))
  (bind _bp_pcs (Variables|Default|GetBP_PCS))
  (bind _returnvalue (Utilities|Array|LastIndex _stack_cws))
  (bind _returnvalue_2 (Pawn|GetControlledPawn _bp_pcs))
  (bind _canremove (Default|OnRemoveCWS RemoveCWS RemoveFromStack RemoveFromParent))
  (if _canremove
    (Utilities|FlowControl|Sequence
      (:then_0
        (if RemoveFromStack
          (bind _returnvalue_3 (Utilities|Array|RemoveItem (Variables|Default|GetStack_CWS) RemoveCWS))
          (if (not _returnvalue_3)
            (CallFunction|AdianPrintError (Utilities|String|Append "Can't find in CWS: " (Utilities|GetDisplayName RemoveCWS))))))
      (:then_1
        (if RemoveFromParent
          (Widget|RemovefromParent RemoveCWS)
          (Class|BPIInputAction|UnbindInputActions(Message) RemoveCWS)))
      (:then_2
        (if (== _returnvalue -1) ; If empty
          (Utilities|IsValid _returnvalue_2
            (:Is%20Valid
              (Input|EnableInput _returnvalue_2 _bp_pcs))
            (:Is%20Not%20Valid
              _))
          (Variables|/Script/Engine.PlayerController|SetbShowMouseCursor (Variables|Default|GetBP_PCS) false)
          (Input|SetInputModeGameOnly (Variables|Default|GetBP_PCS) true)
          (else
            (Class|BPIInputAction|AssignInputActions(Message) (Utilities|Array|Get(acopy) (Variables|Default|GetStack_CWS) _returnvalue))))))))

(fn SetMousetoCenter
  (bind _returnvalue (Viewport|GetViewportSize))
  (Class|PlayerController|SetMouseLocation (Variables|Default|GetBP_PCS) (Math|Float|Truncate (/ (.x _returnvalue) 2.0)) (Math|Float|Truncate (/ (.y _returnvalue) 2.0))))

(fn Warn
  (params (Text :type Text) (ShowTime :type Float%20%28double-precision%29) (OnMouse :type Boolean))
  (bind _returnvalue (UserInterface|CreateWidget "/Game/Widgets/W_Warn.W_Warn_C" (Variables|Default|GetBP_PCS) Text ShowTime OnMouse))
  (UserInterface|Viewport|AddtoViewport _returnvalue 0))

(fn GetPlayerInventory
  (switch Utilities|FlowControl|Switch|SwitchonEPlayerForm (Variables|PlayerForms|GetCurrentPF)
    (:Island
      (return (Variables|/Game/Blueprints/PF_Island.PF_Island_C|GetInventory (Variables|PlayerForms|GetPF_Island))))
    (:Normal
      (return (Variables|/Game/Blueprints/PF_Normal.PF_Normal_C|GetInventory (Variables|PlayerForms|GetPF_Normal))))
    (:Spirit
      (return (Variables|/Game/Blueprints/PF_Normal.PF_Normal_C|GetInventory (Variables|/Game/Blueprints/PF_Spirit.PF_Spirit_C|GetPF_Normal (Variables|PlayerForms|GetPF_Spirit)))))
    (:Dead
      (return (Variables|/Game/Blueprints/PF_Dead.PF_Dead_C|GetInventory (Variables|PlayerForms|GetPF_Dead))))))

(fn SetMouseto
  (params (X :type Float%20%28double-precision%29) (Y :type Float%20%28double-precision%29))
  (bind _returnvalue (Viewport|GetViewportSize))
  (Class|PlayerController|SetMouseLocation (Variables|Default|GetBP_PCS) (Math|Float|Truncate (/ (.x _returnvalue) X)) (Math|Float|Truncate (/ (.y _returnvalue) Y))))

(fn GetBPPAI
  (return self))

(fn GetBPPCS
  (return (Variables|Default|GetBP_PCS)))

(fn GetPlayerForm
  (return (Variables|PlayerForms|GetPF_Island) (Variables|PlayerForms|GetPF_Normal) (Variables|PlayerForms|GetPF_Spirit) (Variables|PlayerForms|GetPF_Dead)))