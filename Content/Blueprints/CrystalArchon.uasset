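; Interactable crystal of an island archon, attached to BPIslandArchon and showing that island's state.
; Server BeginPlay and client OnRep share one setup that binds island events driving crystal scale, essence color, Niagara attractor direction and intact/collapsed visuals and collision.
; Client interaction opens a crystal or non-crystal menu when the player's island matches.
; Server interaction attaches Spirit-form pawns to the island; interruption detaches them.
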(event Custom|OnRep_IslandArchon
  (Utilities|FlowControl|Sequence
    (:then_0
      (Transformation|AttachActorToActor (Variables|Default|GetBP_Island%20Archon) "None" "KeepRelative" "KeepRelative" "KeepRelative" false)
      (EventDispatchers|AssignOnStopIsland (Variables|Default|GetBP_Island%20Archon) (EventDispatchers|CreateEvent :!event OnStopIsland))
      (CallFunction|OnStopIsland)
      (EventDispatchers|AssignOnTargetDirection (Variables|Default|GetBP_Island%20Archon) (EventDispatchers|CreateEvent :!event OnTargetDirection))
      (CallFunction|OnTargetDirection)
      (EventDispatchers|AssignOnEssence (Variables|Default|GetBP_Island%20Archon) (EventDispatchers|CreateEvent :!event OnEssence))
      (CallFunction|OnEssence)
      (EventDispatchers|AssignOnCrystal (Variables|Default|GetBP_Island%20Archon) (EventDispatchers|CreateEvent :!event Custom|OnCrystal_Event))
      (CallFunction|OnCrystalEvent))
    (:then_1
      (EventDispatchers|AssignOnIslandSize (Variables|Default|GetBP_Island%20Archon) (delegate Custom|OnIslandSize_Event)))))

(event Custom|OnIslandSize_Event
  (bind _bp_island_archon (Variables|Default|GetBP_Island%20Archon))
  (bind _bp_island_archon_2 (Variables|Default|GetBP_Island%20Archon))
  (bind _islandsize (Variables|/Script/SkyCraft.Island|GetIslandSize _bp_island_archon))
  (bind _islandsize_2 (Variables|/Script/SkyCraft.Island|GetIslandSize _bp_island_archon_2))
  (bind _returnvalue (* _islandsize_2 2.0))
  (bind _returnvalue_2 (* _islandsize 0.015))
  (bind _returnvalue_3 (+ _returnvalue_2 1.0))
  (bind _returnvalue_4 (+ _returnvalue 1.0))
  (Transformation|SetRelativeScale3D (Variables|Default|GetSM_Crystal) (Math|Vector|MakeVector _returnvalue_4 _returnvalue_4 (+ _returnvalue_4 _returnvalue)))
  (Transformation|SetRelativeScale3D (Variables|Default|GetNS_Crystal) (Math|Vector|MakeVector _returnvalue_3 _returnvalue_3 _returnvalue_3)))

(event Custom|OnCrystal_Event
  (bind _ns_crystal (Variables|Default|GetNS_Crystal))
  (bind _sm_crystal (Variables|Default|GetSM_Crystal))
  (if (Variables|/Script/SkyCraft.Island|GetIslandStarted (Variables|Default|GetBP_Island%20Archon))
    (Variables|/Script/SkyCraft.InteractComponent|SetInteractLocation (Variables|Default|GetInteractSystem) (select (Variables|/Script/SkyCraft.IslandArchon|GetCrystal (Variables|Default|GetBP_Island%20Archon)) "0.000000,0.000000,50.000000" "0, 0, 0"))
    (if (Variables|/Script/SkyCraft.IslandArchon|GetCrystal (Variables|Default|GetBP_Island%20Archon))
      (Components|Activation|SetActive _ns_crystal true false)
      (Rendering|SetVisibility _ns_crystal true false)
      (Collision|SetCollisionEnabled (Variables|Default|GetSM_Crystal) "QueryAndPhysics")
      (Collision|SetCollisionEnabled (Variables|Default|GetCollision_Collapsed) "NoCollision")
      (Components|Activation|SetActive (Variables|Default|GetNS_Collapsed) false false)
      (else
        (Components|Activation|SetActive (Variables|Default|GetNS_Crystal) false false)
        (Rendering|SetVisibility _sm_crystal false false)
        (Collision|SetCollisionEnabled _sm_crystal "NoCollision")
        (Collision|SetCollisionEnabled (Variables|Default|GetCollision_Collapsed) "QueryAndPhysics")
        (Components|Activation|SetActive (Variables|Default|GetNS_Collapsed) true false)))))

(event EventBeginPlay
  (Networking|SwitchHasAuthority
    (:Authority
      (Utilities|FlowControl|Sequence
        (:then_0
          (Transformation|AttachActorToActor (Variables|Default|GetBP_Island%20Archon) "None" "KeepRelative" "KeepRelative" "KeepRelative" false)
          (EventDispatchers|AssignOnStopIsland (Variables|Default|GetBP_Island%20Archon) (EventDispatchers|CreateEvent :!event OnStopIsland))
          (CallFunction|OnStopIsland)
          (EventDispatchers|AssignOnTargetDirection (Variables|Default|GetBP_Island%20Archon) (EventDispatchers|CreateEvent :!event OnTargetDirection))
          (CallFunction|OnTargetDirection)
          (EventDispatchers|AssignOnEssence (Variables|Default|GetBP_Island%20Archon) (EventDispatchers|CreateEvent :!event OnEssence))
          (CallFunction|OnEssence)
          (EventDispatchers|AssignOnCrystal (Variables|Default|GetBP_Island%20Archon) (EventDispatchers|CreateEvent :!event Custom|OnCrystal_Event))
          (CallFunction|OnCrystalEvent))
        (:then_1
          (EventDispatchers|AssignOnIslandSize (Variables|Default|GetBP_Island%20Archon) (delegate Custom|OnIslandSize_Event)))))))

(fn ConstructionScript)

(fn OnRepBPIslandArchon
  (CallFunction|OnRepIslandArchon))

(fn CreateMenu
  (params (Pawn :type Pawn%20Object%20Reference) (BP_PSS :type BP%20PSS%20Object%20Reference))
  (if (Variables|/Script/SkyCraft.IslandArchon|GetCrystal (Variables|Default|GetBP_Island%20Archon))
    (Utilities|IsValid (Variables|Default|GetCWS_Crystal_IslandArchon)
      (:Is%20Valid
        _)
      (:Is%20Not%20Valid
        (bind _returnvalue (UserInterface|CreateWidget "/Game/Widgets/CWS/CWS_Crystal_IslandArchon.CWS_Crystal_IslandArchon_C" 0 (Variables|Default|GetBP_Island%20Archon)))
        (Variables|Default|SetCWS_Crystal_IslandArchon _returnvalue)))
    (Default|ShowMenu (Variables|Default|GetCWS_Crystal_IslandArchon) (EventDispatchers|CreateEvent :!event ShowCompleted))
    (UserInterface|Viewport|AddtoViewport (Variables|Default|GetCWS_Crystal_IslandArchon) 20)
    (Default|AddCWS BP_PSS (Variables|Default|GetCWS_Crystal_IslandArchon) true true true "NewEnumerator2")
    (Default|SetMouseto BP_PSS 2.0 2.0)
    (else
      (Utilities|IsValid (Variables|Default|GetCWS_NonCrystal_IslandArchon)
        (:Is%20Valid
          _)
        (:Is%20Not%20Valid
          (bind _returnvalue_2 (UserInterface|CreateWidget "/Game/Widgets/CWS/CWS_NonCrystal_IslandArchon.CWS_NonCrystal_IslandArchon_C" 0 (Variables|Default|GetBP_Island%20Archon)))
          (Variables|Default|SetCWS_NonCrystal_IslandArchon _returnvalue_2)))
      (Default|ShowMenu (Variables|Default|GetCWS_NonCrystal_IslandArchon))
      (UserInterface|Viewport|AddtoViewport (Variables|Default|GetCWS_NonCrystal_IslandArchon) 20)
      (Default|AddCWS BP_PSS (Variables|Default|GetCWS_NonCrystal_IslandArchon) true true true "NewEnumerator2")
      (Default|SetMouseto BP_PSS 2.0 2.0))))

(fn ShowCompleted)

(fn OnStopIsland
  (CallFunction|OnTargetDirection))

(fn OnTargetDirection
  (bind _bp_island_archon (Variables|Default|GetBP_Island%20Archon))
  (Niagara|SetNiagaraVariable(Vector3) (Variables|Default|GetNS_Crystal) "AttractorPosition" (select (Variables|/Game/Blueprints/BP_IslandArchon.BP_IslandArchon_C|GetStopIsland _bp_island_archon) "0, 0, 0" (* (Variables|/Game/Blueprints/BP_IslandArchon.BP_IslandArchon_C|GetTargetDirection _bp_island_archon) 1e+02))))

(fn OnEssence
  (bind _bp_island_archon (Variables|Default|GetBP_Island%20Archon))
  (bind _essence (Variables|/Game/Blueprints/BP_IslandArchon.BP_IslandArchon_C|GetEssence _bp_island_archon))
  (bind _returnvalue (Class|AdianFL|EssencetoRGB _essence))
  (bind (_r _g _b) (Math|Color|BreakColor _returnvalue))
  (Niagara|SetNiagaraVariable(LinearColor) (Variables|Default|GetNS_Crystal) "EssenceColor" _returnvalue)
  (Rendering|Material|SetVectorParameterValueonMaterials (Variables|Default|GetSM_Crystal) "EssenceColor" (Math|Vector|MakeVector _r _g _b)))

(fn ClientInteractBP
  (params (InteractKey :type EInteractKey%20Enum :default "Interact1") (Pawn :type Pawn%20Object%20Reference) (BP_PSS :type BP%20PSS%20Object%20Reference))
  (if (== (Variables|/Game/Blueprints/BP_PSS.BP_PSS_C|GetBP_IslandArchon BP_PSS) (Variables|Default|GetBP_Island%20Archon))
    (CallFunction|CreateMenu Pawn BP_PSS)
    (return true)))

(fn ClientInterruptBP
  (params (InterruptedBy :type EInterruptedBy%20Enum :default "Player") (InteractKey :type EInteractKey%20Enum :default "Interact1") (Pawn :type Pawn%20Object%20Reference) (BP_PSS :type BP%20PSS%20Object%20Reference))
  (return false))

(fn ServerInteractBP
  (params (InteractKey :type EInteractKey%20Enum :default "Interact1") (Pawn :type Pawn%20Object%20Reference) (BP_PSS :type BP%20PSS%20Object%20Reference))
  (switch Utilities|FlowControl|Switch|SwitchonEPlayerForm (Variables|/Script/SkyCraft.PSS|GetPlayerForm BP_PSS)
    (:Normal
      (return true))
    (:Spirit
      (Transformation|AttachActorToActor Pawn (Variables|Default|GetBP_Island%20Archon) "None" "KeepWorld" "KeepWorld" "KeepWorld" true)
      (return true))))

(fn ServerInterruptBP
  (params (InterruptedBy :type EInterruptedBy%20Enum :default "Player") (InteractKey :type EInteractKey%20Enum :default "Interact1") (Pawn :type Pawn%20Object%20Reference) (BP_PSS :type BP%20PSS%20Object%20Reference))
  (switch Utilities|FlowControl|Switch|SwitchonEPlayerForm (Variables|/Script/SkyCraft.PSS|GetPlayerForm BP_PSS)
    (:Normal
      (return true))
    (:Spirit
      (Transformation|DetachFromActor Pawn "KeepWorld" "KeepWorld" "KeepWorld")
      (return true))))