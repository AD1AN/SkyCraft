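; ItemDrop is an interactable world pickup holding an inventory, destroyed when removals empty it.
; On hit it stops physics, floats and attaches to any IslandArchon struck.
; The server merges overlapping drops by Priority, breaking ties by distance from world origin.
; Normal pawns take single stacks directly or open a widget for several; Spirits get their own widget and can drag the drop on a Tick-driven tether via multicast start/stop.
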(event OnComponentBeginOverlap(SphereMerge)
  (params (OverlappedComponent :type Primitive%20Component%20Object%20Reference) (OtherActor :type Actor%20Object%20Reference) (OtherComp :type Primitive%20Component%20Object%20Reference) (OtherBodyIndex :type Integer) (bFromSweep :type Boolean) (SweepResult :type Hit%20Result%20Structure%20%28by%20ref%29))
  (if (Networking|IsServer)
    (bind _asitem_drop (Utilities|Casting|CastToItemDrop OtherActor))
    (Variables|Default|SetOverlapped%20Item%20Drop _asitem_drop)
    (if (== (Variables|Default|GetPriority) (Variables|ItemDrop_C|GetPriority (Variables|Default|GetOverlapped%20Item%20Drop)))
      (if (> (Math|Vector|Distance(Vector) (Transformation|GetActorLocation) "0, 0, 0") (Math|Vector|Distance(Vector) (Transformation|GetActorLocation (Variables|Default|GetOverlapped%20Item%20Drop)) "0, 0, 0"))
        (for _array_element (Variables|/Game/Blueprints/Inventory.Inventory_C|GetSlots (Variables|ItemDrop_C|GetInventory (Variables|Default|GetOverlapped%20Item%20Drop))) :!label _label ; Consume overlapped ItemDrop to this
          (Default|MulticastADDInventory (Variables|Default|GetInventory) _array_element))
        (Actor|DestroyActor (Variables|Default|GetOverlapped%20Item%20Drop)))
      (elif (> (Variables|Default|GetPriority) (Variables|ItemDrop_C|GetPriority (Variables|Default|GetOverlapped%20Item%20Drop)))
        (goto _label)))))

(event Custom|REMOVE_Inventory_Event_0
  (params (RemovedIndex :type Integer))
  (if (<= (Utilities|Array|Length (Variables|/Game/Blueprints/Inventory.Inventory_C|GetSlots (Variables|Default|GetInventory))) 0)
    (Actor|DestroyActor)))

(event Custom|StartIdle
  (bind _z (Timeline|IdleFloating Play)
    (:Update
      (Transformation|AddActorLocalOffset (Math|Vector|MakeVector 0.0 0.0 (* _z (Utilities|Time|GetWorldDeltaSeconds) 4e+01)) false false))))

(event Custom|OnDestroyed_Event_1
  (params (DestroyedActor :type Actor%20Object%20Reference))
  ;[0.6159 1 0.7401 1 125] Start Drag (Not Initial)
  (CallFunction|MulticastStopDrag)
  (Variables|Default|SetDrag_PF_Spirit 0) ; empty
)

(event Collision|EventHit
  (params (MyComp :type Primitive%20Component%20Object%20Reference) (Other :type Actor%20Object%20Reference) (OtherComp :type Primitive%20Component%20Object%20Reference) (bSelfMoved :type Boolean) (HitLocation :type Vector :default "0, 0, 0") (HitNormal :type Vector :default "0, 0, 0") (NormalImpulse :type Vector :default "0, 0, 0") (Hit :type Hit%20Result%20Structure%20%28by%20ref%29))
  (if (Networking|IsServer)
    (bind _rootactor (CallFunction|GetRootActor Other))
    (Variables|Default|SetPriority 1)
    (CallFunction|StartIdle)
    (Physics|SetSimulatePhysics (Variables|Default|GetStaticMesh) false)
    (bind _asisland_archon (Utilities|Casting|CastToIslandArchon _rootactor))
    (bind _output_get (Variables|Default|SetAttachedToIA _asisland_archon))
    (Transformation|AttachActorToActor _output_get "None" "KeepWorld" "KeepWorld" "KeepWorld" false)))

(event EventTick
  (params (DeltaSeconds :type Float%20%28single-precision%29))
  (if (> (Transformation|GetDistanceTo (Variables|Default|GetDrag_PF_Spirit)) 7e+01)
    (Transformation|SetActorLocation (+ (Transformation|GetActorLocation (Variables|Default|GetDrag_PF_Spirit)) (* (Math|Vector|GetForwardVector (Math|Rotator|FindLookatRotation (Transformation|GetActorLocation (Variables|Default|GetDrag_PF_Spirit)) (Transformation|GetActorLocation))) 70)) false false)))

(event EventSetDragChar
  (params (DragChar :type Actor%20Object%20Reference))
  (bind _aspf_spirit (Utilities|Casting|CastToPF_Spirit DragChar)
    (:then
      (Variables|Default|SetDrag_PF_Spirit _aspf_spirit))
    (:CastFailed
      (Variables|Default|SetDrag_PF_Spirit 0))))

(event EventBeginPlay
  (if (Networking|IsServer)
    (EventDispatchers|AssignREMOVEInventory (Variables|Default|GetInventory) (delegate Custom|REMOVE_Inventory_Event_0))
    (Utilities|FlowControl|Delay 0.15)
    (Collision|SetCollisionEnabled (Variables|Default|GetSphereMerge) "QueryOnly")))

(event EventMulticastStartDrag
  ;[0.6159 1 0.7401 1 125] Start Drag (Not Initial)
  (Transformation|DetachFromActor "KeepWorld" "KeepWorld" "KeepWorld")
  (Collision|SetCollisionEnabled (Variables|Default|GetSphereMerge) "NoCollision")
  (Collision|SetCollisionEnabled (Variables|Default|GetStaticMesh) "NoCollision")
  (Variables|/Script/SkyCraft.InteractSystem|SetbInteractable (Variables|Default|GetInteractSystem) false)
  (Actor|Tick|SetActorTickEnabled true)
  (if (Networking|IsServer)
    (Game|AssignOnDestroyed (Variables|Default|GetDrag_PF_Spirit) (delegate Custom|OnDestroyed_Event_1))))

(event EventMulticastStopDrag
  ;[1 0.4366 0.4665 1 125] Stop Drag
  (Utilities|IsValid (Variables|/Game/Blueprints/PF_Spirit.PF_Spirit_C|GetAttachedToIA (Variables|Default|GetDrag_PF_Spirit))
    (:Is%20Valid
      (Transformation|AttachActorToActor (Variables|/Game/Blueprints/PF_Spirit.PF_Spirit_C|GetAttachedToIA (Variables|Default|GetDrag_PF_Spirit)) "None" "KeepWorld" "KeepWorld" "KeepWorld" true))
    (:Is%20Not%20Valid
      _))
  (Collision|SetCollisionEnabled (Variables|Default|GetStaticMesh) "QueryAndPhysics")
  (Variables|/Script/SkyCraft.InteractSystem|SetbInteractable (Variables|Default|GetInteractSystem) true)
  (Actor|Tick|SetActorTickEnabled false)
  (Game|UnbindEventfromOnDestroyed (Variables|Default|GetDrag_PF_Spirit) (delegate Custom|OnDestroyed_Event_1)))

(fn ConstructionScript)

(fn TryGetIDIA
  (bind _attachedtoia (Variables|Default|GetAttachedToIA))
  (Utilities|IsValid _attachedtoia
    (:Is%20Valid
      (return (Variables|/Game/Blueprints/IslandArchon.IslandArchon_C|GetID_IA _attachedtoia)))
    (:Is%20Not%20Valid
      (return -1))))

(fn ClientInteractBP
  (params (InteractKey :type EInteractKey%20Enum :default "Interact1") (Pawn :type Pawn%20Object%20Reference) (BP_PAI :type BP%20PAI%20Object%20Reference))
  (switch Utilities|FlowControl|Switch|SwitchonEInteractKey InteractKey
    (:Interact1
      (switch Utilities|FlowControl|Switch|SwitchonEPlayerForm (Variables|/Game/Blueprints/BP_PAI.BP_PAI_C|GetCurrentPF BP_PAI)
        (:Normal
          (if (> (Utilities|Array|Length (Variables|/Game/Blueprints/Inventory.Inventory_C|GetSlots (Variables|Default|GetInventory))) 1)
            (bind _returnvalue (UserInterface|CreateWidget "/Game/Widgets/CWS/CWS_ItemDrop_Normal.CWS_ItemDrop_Normal_C" 0 self Pawn))
            (UserInterface|Viewport|AddtoViewport _returnvalue 10)
            (Default|AddCWS BP_PAI _returnvalue true true "NewEnumerator2")))
        (:Spirit
          (bind _returnvalue_2 (UserInterface|CreateWidget "/Game/Widgets/CWS/CWS_ItemDrop_Spirit.CWS_ItemDrop_Spirit_C" 0 self Pawn))
          (UserInterface|Viewport|AddtoViewport _returnvalue_2 0)
          (Default|AddCWS BP_PAI _returnvalue_2 true true "NewEnumerator2")
          (return false))))))

(fn ClientInterruptBP
  (params (InterruptedBy :type EInterruptedBy%20Enum :default "Player") (InteractKey :type EInteractKey%20Enum :default "Interact1") (Pawn :type Pawn%20Object%20Reference) (BP_PAI :type BP%20PAI%20Object%20Reference))
  (return false))

(fn GetInventory
  (return (Variables|Default|GetInventory)))

(fn GetInteractLocation
  (return (Transformation|GetActorLocation)))

(fn GetInteractSystem
  (return (Variables|Default|GetInteractSystem)))

(fn ServerInteractBP
  (params (InteractKey :type EInteractKey%20Enum :default "Interact1") (Pawn :type Pawn%20Object%20Reference) (BP_PAI :type BP%20PAI%20Object%20Reference))
  (bind _inventory (Variables|Default|GetInventory))
  (bind _slots (Variables|/Game/Blueprints/Inventory.Inventory_C|GetSlots _inventory))
  (bind _output (Utilities|Array|Get(acopy) _slots))
  (switch Utilities|FlowControl|Switch|SwitchonEInteractKey InteractKey
    (:Interact1
      (switch Utilities|FlowControl|Switch|SwitchonEPlayerForm (Variables|/Game/Blueprints/BP_PAI.BP_PAI_C|GetCurrentPF BP_PAI)
        (:Normal
          (bind _inventory_2 (Class|BPIGetInventory|GetInventory(Message) Pawn))
          (LocalVariables|Set_Inventory _inventory_2)
          (if (not (> (Utilities|Array|Length (Variables|/Game/Blueprints/Inventory.Inventory_C|GetSlots (Variables|Default|GetInventory))) 1))
            (bind (_success _unsuccessquantity) (Default|AddtoInventory (LocalVariables|Get_Inventory) (Utilities|Array|Get(acopy) (Variables|/Game/Blueprints/Inventory.Inventory_C|GetSlots (Variables|Default|GetInventory)))))
            (if _success
              (Actor|DestroyActor)
              (else
                (Utilities|Array|SetArrayElem _slots 0 (Utilities|Struct|MakeInventorySlot (.da_item _output) _unsuccessquantity (.properties _output)))))))
        (:Spirit
          (return false))))
    (:Interact3
      (switch Utilities|FlowControl|Switch|SwitchonEPlayerForm (Variables|/Game/Blueprints/BP_PAI.BP_PAI_C|GetCurrentPF BP_PAI)
        (:Normal
          (return false))
        (:Spirit
          (Default|ServerStartDrag (Variables|/Game/Blueprints/PF_Normal.PF_Normal_C|GetPF_Spirit (Variables|/Game/Blueprints/BP_PAI.BP_PAI_C|GetPF_Normal BP_PAI)) self)
          (return false))))))

(fn ServerInterruptBP
  (params (InterruptedBy :type EInterruptedBy%20Enum :default "Player") (InteractKey :type EInteractKey%20Enum :default "Interact1") (Pawn :type Pawn%20Object%20Reference) (BP_PAI :type BP%20PAI%20Object%20Reference))
  (return false))