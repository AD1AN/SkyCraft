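; Server-side actor component that streams Essence chunks around its owner in the Sky Main level.
; When the owner crosses a chunk boundary, it releases chunks outside a circular render range and claims or spawns those inside.
; GM_Sky holds the shared chunk registry, and each generator increments or decrements a chunk's HMPR reference count instead of destroying it.
; Helper functions release all held chunks or copy another generator's chunk state.
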(event EventBeginPlay
  (Variables|Default|SetActor (Components|GetOwner))
  (bind _sgi (Class|BPISGI|GetSGI(Message) (Game|GetGameInstance)))
  (Variables|Default|SetSGI _sgi)
  (if (Networking|IsServer)
    (switch Utilities|FlowControl|Switch|SwitchonCurrentLevel (Variables|/Game/Blueprints/SGI.SGI_C|GetCurrentLevel (Variables|Default|GetSGI))
      (:NewEnumerator1
        (if (Class|LowEntryExtendedStandardLibrary|ShippingBuild)
          _
          (else
            (Variables|Default|SetShippingRenderRangeXY (Variables|Default|GetTestRenderRangeXY))))
        (bind _asgm_sky (Utilities|Casting|CastToGM_Sky (Game|GetGameMode)))
        (Variables|Default|SetGM_Sky _asgm_sky)
        (Components|Tick|SetComponentTickEnabled true)))))

(event EventTick
  (params (DeltaSeconds :type Float%20%28single-precision%29))
  (bind (_x _y) (CallFunction|GetActorChunkCors))
  (bind (_x_2 _y_2) (CallFunction|GetActorChunkCors))
  (if (not (and (== _x_2 (.x (Variables|Default|GetLastActorChunkCors))) (== _y_2 (.y (Variables|Default|GetLastActorChunkCors))))) ; Player has changed Chunk Coordinates
    (Variables|Default|SetLastActorChunkCors (Utilities|Struct|MakeIntVector _x _y 0))
    (CallFunction|DestroyChunks)
    (CallFunction|SpawnChunks)))

(fn GetActorChunkCors
  (bind _actor (Variables|Default|GetActor))
  (bind _chunksizexy (Variables|Default|GetChunkSizeXY))
  (bind _returnvalue (Transformation|GetActorLocation _actor))
  (bind _returnvalue_2 (/ _returnvalue _chunksizexy))
  (bind (_x _y) (Math|Vector|BreakVector _returnvalue_2))
  (return (Math|Float|Round _x) (Math|Float|Round _y)))

(fn DestroyChunks
  (bind (_x _y) (CallFunction|GetActorChunkCors))
  (bind _chunksizexy (Variables|Default|GetChunkSizeXY))
  (bind _chunksizexy_2 (Variables|Default|GetChunkSizeXY))
  (for (_array_element _array_index) (Variables|Default|GetHMPR_SpawnedChunkEssenceCors)
    (LocalVariables|SetTempIndex _array_index)
    (if (>= (Math|Vector|Distance(Vector) (Math|Vector|MakeVector (* (.X (Utilities|Struct|BreakIntVector _array_element)) _chunksizexy) (* (.Y (Utilities|Struct|BreakIntVector _array_element)) _chunksizexy) 0.0) (Math|Vector|MakeVector (* _x _chunksizexy_2) (* _y _chunksizexy_2) 0.0)) (* (Variables|Default|GetShippingRenderRangeXY) (Variables|Default|GetChunkSizeXY)))
      (Utilities|Array|Add (LocalVariables|GetIndexForRemoval) (LocalVariables|GetTempIndex))))
  (for (_array_element_2 _array_index_2) (LocalVariables|GetIndexForRemoval)
    (Variables|/Game/Blueprints/SkyMain/SA_Chunk_Essence.SA_Chunk_Essence_C|SetHMPR (Utilities|Array|Get(acopy) (Variables|Default|GetHMPR_SpawnedChunkEssence) (- _array_element_2 _array_index_2)) (- (Variables|/Game/Blueprints/SkyMain/SA_Chunk_Essence.SA_Chunk_Essence_C|GetHMPR (Utilities|Array|Get(acopy) (Variables|Default|GetHMPR_SpawnedChunkEssence) (- _array_element_2 _array_index_2))) 1))
    (Utilities|Array|RemoveIndex (Variables|Default|GetHMPR_SpawnedChunkEssenceCors) (- _array_element_2 _array_index_2))
    (Utilities|Array|RemoveIndex (Variables|Default|GetHMPR_SpawnedChunkEssence) (- _array_element_2 _array_index_2))))

(fn SpawnChunks
  (bind (_x _y) (CallFunction|GetActorChunkCors))
  (bind _shippingrenderrangexy (Variables|Default|GetShippingRenderRangeXY))
  (bind _shippingrenderrangexy_2 (Variables|Default|GetShippingRenderRangeXY))
  (bind _chunksizexy (Variables|Default|GetChunkSizeXY))
  (bind _gm_sky (Variables|Default|GetGM_Sky))
  (bind _gm_sky_2 (Variables|Default|GetGM_Sky))
  (bind _chunksizexy_2 (Variables|Default|GetChunkSizeXY))
  (for _index (range (* _shippingrenderrangexy_2 -1) _shippingrenderrangexy_2)
    (LocalVariables|SetTempX _index)
    (for _index_2 (range (* _shippingrenderrangexy -1) _shippingrenderrangexy)
      (LocalVariables|SetTempY _index_2)
      (LocalVariables|SetChunkCors (Utilities|Struct|MakeIntVector (+ _x (LocalVariables|GetTempX)) (+ _y (LocalVariables|GetTempY))))
      (if (and (not (Utilities|Array|ContainsItem (Variables|Default|GetHMPR_SpawnedChunkEssenceCors) (LocalVariables|GetChunkCors))) (< (Math|Vector|VectorLength (Math|Vector|MakeVector (* (LocalVariables|GetTempX) _chunksizexy) (* (LocalVariables|GetTempY) _chunksizexy) 0.0)) (* (Variables|Default|GetShippingRenderRangeXY) (Variables|Default|GetChunkSizeXY))))
        (if (Utilities|Array|ContainsItem (Variables|/Game/Blueprints/SkyMain/GM_Sky.GM_Sky_C|GetSpawnedChunkEssenceCors (Variables|Default|GetGM_Sky)) (LocalVariables|GetChunkCors))
          (Utilities|Array|Add (Variables|Default|GetHMPR_SpawnedChunkEssenceCors) (LocalVariables|GetChunkCors))
          (Utilities|Array|Add (Variables|Default|GetHMPR_SpawnedChunkEssence) (Utilities|Array|Get(acopy) (Variables|/Game/Blueprints/SkyMain/GM_Sky.GM_Sky_C|GetSpawnedChunkEssence _gm_sky_2) (Utilities|Array|FindItem (Variables|/Game/Blueprints/SkyMain/GM_Sky.GM_Sky_C|GetSpawnedChunkEssenceCors _gm_sky_2) (LocalVariables|GetChunkCors))))
          (Variables|/Game/Blueprints/SkyMain/SA_Chunk_Essence.SA_Chunk_Essence_C|SetHMPR (Utilities|Array|Get(acopy) (Variables|/Game/Blueprints/SkyMain/GM_Sky.GM_Sky_C|GetSpawnedChunkEssence _gm_sky_2) (Utilities|Array|FindItem (Variables|/Game/Blueprints/SkyMain/GM_Sky.GM_Sky_C|GetSpawnedChunkEssenceCors _gm_sky_2) (LocalVariables|GetChunkCors))) (+ (Variables|/Game/Blueprints/SkyMain/SA_Chunk_Essence.SA_Chunk_Essence_C|GetHMPR (Utilities|Array|Get(acopy) (Variables|/Game/Blueprints/SkyMain/GM_Sky.GM_Sky_C|GetSpawnedChunkEssence _gm_sky_2) (Utilities|Array|FindItem (Variables|/Game/Blueprints/SkyMain/GM_Sky.GM_Sky_C|GetSpawnedChunkEssenceCors _gm_sky_2) (LocalVariables|GetChunkCors)))) 1))
          (else
            ;[1 1 1] SpawnChunk
            (bind _returnvalue (Game|SpawnActorfromClass "/Game/Blueprints/SkyMain/SA_Chunk_Essence.SA_Chunk_Essence_C" (Math|Transform|MakeTransform (Math|Vector|MakeVector (* (.x (LocalVariables|GetChunkCors)) _chunksizexy_2) (* (.y (LocalVariables|GetChunkCors)) _chunksizexy_2) 5e+03) "0, 0, 0" "1.000000,1.000000,1.000000") "AlwaysSpawn" 0 (Variables|Default|GetGM_Sky) 1 0))
            (Utilities|Array|Add (Variables|/Game/Blueprints/SkyMain/GM_Sky.GM_Sky_C|GetSpawnedChunkEssence _gm_sky) _returnvalue)
            (Utilities|Array|Add (Variables|/Game/Blueprints/SkyMain/GM_Sky.GM_Sky_C|GetSpawnedChunkEssenceCors _gm_sky) (LocalVariables|GetChunkCors))
            (Utilities|Array|Add (Variables|Default|GetHMPR_SpawnedChunkEssence) _returnvalue)
            (Utilities|Array|Add (Variables|Default|GetHMPR_SpawnedChunkEssenceCors) (LocalVariables|GetChunkCors))))))))

(fn MinusSpawnedChunks
  (for _array_element (Variables|Default|GetHMPR_SpawnedChunkEssence)
    (Variables|/Game/Blueprints/SkyMain/SA_Chunk_Essence.SA_Chunk_Essence_C|SetHMPR _array_element (- (Variables|/Game/Blueprints/SkyMain/SA_Chunk_Essence.SA_Chunk_Essence_C|GetHMPR _array_element) 1)))
  (Utilities|Array|Clear (Variables|Default|GetHMPR_SpawnedChunkEssence))
  (Utilities|Array|Clear (Variables|Default|GetHMPR_SpawnedChunkEssenceCors)))

(fn TransferChunks
  (params (FromGenerator :type Generator%20Essence%20Object%20Reference))
  (Variables|Default|SetHMPR_SpawnedChunkEssence (Variables|Generator_Essence_C|GetHMPR_SpawnedChunkEssence FromGenerator))
  (Variables|Default|SetHMPR_SpawnedChunkEssenceCors (Variables|Generator_Essence_C|GetHMPR_SpawnedChunkEssenceCors FromGenerator))
  (Variables|Default|SetLastActorChunkCors (Variables|Generator_Essence_C|GetLastActorChunkCors FromGenerator))
  (return))