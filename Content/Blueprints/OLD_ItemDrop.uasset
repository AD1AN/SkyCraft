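; Dropped item actor (named OLD) that Normal pawns can pick up and Spirit pawns can drag.
; Server interaction adds the slot to the pawn's inventory, destroying the actor or updating its quantity, or starts a Spirit drag.
; Multicast drag events toggle collision, interactability and tick, detaching on start and attaching to the Spirit's AttachedToIA on stop.
; The server binds the Spirit's OnDestroyed to end the drag.
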(event Custom|OnDestroyed_Event_1
  (params (DestroyedActor :type Actor%20Object%20Reference))
  ;[0.6159 1 0.7401 1 125] Start Drag (Not Initial)
  (CallFunction|MulticastStopDrag)
  (Variables|Default|SetDrag_PF_Spirit 0) ; empty
)

(event EventSetDragChar
  (params (DragChar :type Actor%20Object%20Reference))
  (bind _aspf_spirit (Utilities|Casting|CastToPF_Spirit DragChar)
    (:then
      (Variables|Default|SetDrag_PF_Spirit _aspf_spirit))
    (:CastFailed
      (Variables|Default|SetDrag_PF_Spirit 0))))

(event EventMulticastStartDrag
  ;[0.6159 1 0.7401 1 125] Start Drag (Not Initial)
  (Transformation|DetachFromActor "KeepWorld" "KeepWorld" "KeepWorld")
  (Collision|SetCollisionEnabled (Variables|Default|GetStaticMesh) "NoCollision")
  (Variables|/Script/SkyCraft.InteractSystem|SetbInteractable (Variables|Default|GetInteractSystem) false)
  (Actor|Tick|SetActorTickEnabled true)
  (if (Networking|IsServer)
    (Game|AssignOnDestroyed (Variables|Default|GetDrag_PF_Spirit) (delegate Custom|OnDestroyed_Event_1))))

(event EventMulticastStopDrag
  ;[1 0.4366 0.4665 1 125] Stop Drag
  (Utilities|IsValid (Variables|/Game/Blueprints/PF_Spirit.PF_Spirit_C|GetAttachedToIA (Variables|Default|GetDrag_PF_Spirit))
    (:Is%20Valid
      (Transformation|AttachActorToActor (Variables|/Game/Blueprints/PF_Spirit.PF_Spirit_C|GetAttachedToIA (Variables|Default|GetDrag_PF_Spirit)) "None" "KeepWorld" "KeepWorld" "KeepWorld" true))
    (:Is%20Not%20Valid
      _))
  (Collision|SetCollisionEnabled (Variables|Default|GetStaticMesh) "QueryAndPhysics")
  (Variables|/Script/SkyCraft.InteractSystem|SetbInteractable (Variables|Default|GetInteractSystem) true)
  (Actor|Tick|SetActorTickEnabled false)
  (Game|UnbindEventfromOnDestroyed (Variables|Default|GetDrag_PF_Spirit) (delegate Custom|OnDestroyed_Event_1)))

(fn ConstructionScript)

(fn TryGetIDIA
  (bind _attachedtoia (Variables|Default|GetAttachedToIA))
  (Utilities|IsValid _attachedtoia
    (:Is%20Valid
      (return (Variables|/Game/Blueprints/IslandArchon.IslandArchon_C|GetID_IA _attachedtoia)))
    (:Is%20Not%20Valid
      (return -1))))

(fn ClientInteractBP
  (params (InteractKey :type EInteractKey%20Enum :default "Interact1") (Pawn :type Pawn%20Object%20Reference) (BP_PAI :type BP%20PAI%20Object%20Reference))
  (return false))

(fn ClientInterruptBP
  (params (InterruptedBy :type EInterruptedBy%20Enum :default "Player") (InteractKey :type EInteractKey%20Enum :default "Interact1") (Pawn :type Pawn%20Object%20Reference) (BP_PAI :type BP%20PAI%20Object%20Reference))
  (return false))

(fn GetInventory
  (return 0))

(fn ServerInteractBP
  (params (InteractKey :type EInteractKey%20Enum :default "Interact1") (Pawn :type Pawn%20Object%20Reference) (BP_PAI :type BP%20PAI%20Object%20Reference))
  (switch Utilities|FlowControl|Switch|SwitchonEInteractKey InteractKey
    (:Interact1
      (switch Utilities|FlowControl|Switch|SwitchonEPlayerForm (Variables|/Game/Blueprints/BP_PAI.BP_PAI_C|GetCurrentPF BP_PAI)
        (:Normal
          (bind _inventory (Class|BPIGetInventory|GetInventory(Message) Pawn))
          (LocalVariables|Set_Inventory _inventory)
          (bind (_success _quantity) (Default|Add (LocalVariables|Get_Inventory) (Variables|Default|GetInventorySlot)))
          (if _success
            (Actor|DestroyActor)
            (else
              (Variables|Default|SetInventorySlot (Utilities|Struct|MakeInventorySlot (.da_item (Variables|Default|GetInventorySlot)) _quantity (.properties (Variables|Default|GetInventorySlot)))))))))
    (:Interact3
      (switch Utilities|FlowControl|Switch|SwitchonEPlayerForm (Variables|/Game/Blueprints/BP_PAI.BP_PAI_C|GetCurrentPF BP_PAI)
        (:Spirit
          (Default|ServerStartDrag (Variables|/Game/Blueprints/PF_Normal.PF_Normal_C|GetPF_Spirit (Variables|/Game/Blueprints/BP_PAI.BP_PAI_C|GetPF_Normal BP_PAI)) self)
          (return true))))))

(fn ServerInterruptBP
  (params (InterruptedBy :type EInterruptedBy%20Enum :default "Player") (InteractKey :type EInteractKey%20Enum :default "Interact1") (Pawn :type Pawn%20Object%20Reference) (BP_PAI :type BP%20PAI%20Object%20Reference))
  (return false))