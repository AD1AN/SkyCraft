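; BP_SingleStone is an interactable stone that turns into a Stone item drop when a pawn interacts with it.
; The server interact handler spawns an OLD_ItemDrop slightly above the actor, pops it upward with a velocity-change impulse, then destroys the stone.
; Client interact and both interrupt handlers just return false, and the event graph is unused.
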(event EventBeginPlay)

(event Collision|EventActorBeginOverlap
  (params (OtherActor :type Actor%20Object%20Reference)))

(event EventTick
  (params (DeltaSeconds :type Float%20%28single-precision%29)))

(fn ConstructionScript)

(fn ClientInteractBP
  (params (InteractKey :type EInteractKey%20Enum :default "Interact1") (Pawn :type Pawn%20Object%20Reference) (BP_PAI :type BP%20PAI%20Object%20Reference))
  (return false))

(fn ClientInterruptBP
  (params (InterruptedBy :type EInterruptedBy%20Enum :default "Player") (InteractKey :type EInteractKey%20Enum :default "Interact1") (Pawn :type Pawn%20Object%20Reference) (BP_PAI :type BP%20PAI%20Object%20Reference))
  (return false))

(fn ServerInteractBP
  (params (InteractKey :type EInteractKey%20Enum :default "Interact1") (Pawn :type Pawn%20Object%20Reference) (BP_PAI :type BP%20PAI%20Object%20Reference))
  (bind _returnvalue (Game|SpawnActorfromClass "/Game/Blueprints/OLD_ItemDrop.OLD_ItemDrop_C" (Math|Transform|MakeTransform (+ (Transformation|GetActorLocation) "0.000000,0.000000,25.000000") "0, 0, 0" "1.000000,1.000000,1.000000") "AlwaysSpawn" "MultiplyWithRoot" 0 (Utilities|Struct|MakeInventorySlot "/Game/DataAssets/Item/Stone.Stone" 1 0) 0))
  (Physics|AddImpulse (Variables|/Game/Blueprints/OLD_ItemDrop.OLD_ItemDrop_C|GetStaticMesh _returnvalue) "0.000000,0.000000,200.000000" "None" true)
  (Actor|DestroyActor)
  (return true))

(fn ServerInterruptBP
  (params (InterruptedBy :type EInterruptedBy%20Enum :default "Player") (InteractKey :type EInteractKey%20Enum :default "Interact1") (Pawn :type Pawn%20Object%20Reference) (BP_PAI :type BP%20PAI%20Object%20Reference))
  (return false))