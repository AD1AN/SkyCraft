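; PingCheck is a component that measures the round-trip time between client and server in milliseconds.
; On BeginPlay, the server tells the client to enable component tick.
; Tick accumulates delta time and keeps one server request in flight, which the server answers with a client event.
; That response stores the elapsed time in EndMS and resets for the next probe, so resolution is limited to frame time.
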(event Custom|Server_GiveResponse
  (CallFunction|ClientTakeResponse))

(event Custom|Client_TakeResponse
  (Variables|Default|SetEndMS (Variables|Default|GetMS))
  (Variables|Default|SetMS 0.0)
  (Variables|Default|SetSent false))

(event Custom|Client_EnableTick
  (Components|Tick|SetComponentTickEnabled true))

(event EventTick
  (params (DeltaSeconds :type Float%20%28single-precision%29))
  (Variables|Default|SetMS (+ (* DeltaSeconds 1e+03) (Variables|Default|GetMS)))
  (if (not (Variables|Default|GetSent))
    (Variables|Default|SetSent true)
    (CallFunction|ServerGiveResponse)))

(event EventBeginPlay
  (if (Networking|IsServer)
    (CallFunction|ClientEnableTick)))