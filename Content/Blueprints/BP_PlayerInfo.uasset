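; Per-player info actor that links its owning Sky player controller to that player's forms (Island, Normal, Spirit, Dead) and Island Archon.
; Initializes once, caching game instance, controller and, on the server, game mode; the owning client registers it with the game instance.
; Multicast events update form and archon references, while server events relay chat and handle island-pawn possession and Essence transfers.
; Chat input and display go through the Normal form's widget.
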(event Custom|Server_StopIA
  (Default|StopIA (Variables|Default|GetIslandArchon)))

(event Custom|Multicast_SetIslandArchon
  (params (IslandArchon :type Island%20Archon%20Object%20Reference))
  (bind _bp_playercontroller (Variables|Default|GetBP_PlayerController))
  (bind _output_get (Variables|Default|SetIslandArchon IslandArchon))
  (Utilities|IsValid _bp_playercontroller
    (:Is%20Valid
      (Variables|/Game/Blueprints/BP_PlayerController.BP_PlayerController_C|SetIslandArchon _bp_playercontroller _output_get))))

(event Custom|Multicast_Init
  (if (not (Variables|Default|GetInitialized))
    (Variables|Default|SetInitialized true)
    (bind _assgi (Utilities|Casting|CastToSGI (Game|GetGameInstance))
      (:then
        _)
      (:CastFailed
        _))
    (Variables|Default|SetSGI _assgi)
    (bind _pc_sky (Class|BPIPSky|GetPCSky(Message) (Components|GetOwner)))
    (Variables|Default|SetBP_PlayerController _pc_sky)
    (Utilities|IsOwner
      (:Server
        (bind _asgm_sky (Utilities|Casting|CastToGM_Sky (Game|GetGameMode)))
        (Variables|Default|SetGM_Sky _asgm_sky))
      (:OwningClient
        (Variables|/Game/Blueprints/SGI.SGI_C|SetPP_Sky (Variables|Default|GetSGI) self)))))

(event Custom|EnsureInit
  (if (not (Variables|Default|GetInitialized))
    (Variables|Default|SetInitialized true)
    (bind _assgi (Utilities|Casting|CastToSGI (Game|GetGameInstance))
      (:then
        _)
      (:CastFailed
        _))
    (Variables|Default|SetSGI _assgi)
    (bind _pc_sky (Class|BPIPSky|GetPCSky(Message) (Components|GetOwner)))
    (Variables|Default|SetBP_PlayerController _pc_sky)
    (Utilities|IsOwner
      (:Server
        (bind _asgm_sky (Utilities|Casting|CastToGM_Sky (Game|GetGameMode)))
        (Variables|Default|SetGM_Sky _asgm_sky))
      (:OwningClient
        (Variables|/Game/Blueprints/SGI.SGI_C|SetPP_Sky (Variables|Default|GetSGI) self)))))

(event Custom|Server_IA_GiveEssence
  (params (GiveEssence :type S%20Essence%20Structure))
  (Variables|/Game/Blueprints/IslandArchon.IslandArchon_C|SetEssence (Variables|Default|GetIslandArchon) (CallFunction|AddEssence GiveEssence (Variables|/Game/Blueprints/IslandArchon.IslandArchon_C|GetEssence (Variables|Default|GetIslandArchon))))
  (Variables|/Game/Blueprints/PF_Normal.PF_Normal_C|SetEssence (Variables|PlayerForms|GetPF_Normal) (CallFunction|SubtractEssence (Variables|/Game/Blueprints/PF_Normal.PF_Normal_C|GetEssence (Variables|PlayerForms|GetPF_Normal)) GiveEssence)))

(event Custom|Server_SendMessage
  (params (Sender :type String) (Message :type String))
  ;[1 1 1] Chat
  (Default|SendMessagetoEveryone (Variables|Default|GetGM_Sky) Sender Message))

(event Custom|AddMessageToChat
  (params (Sender :type String) (Message :type String))
  ;[1 1 1] Chat
  (Default|AddMessagetoChat (Variables|/Game/Blueprints/PF_Normal.PF_Normal_C|GetW_PF_Normal (Variables|PlayerForms|GetPF_Normal)) Sender Message))

(event Custom|Multicast_PlayerForm_Possessed
  (params (CurrentPlayerForm :type EPlayerForm%20Enum :default "Island") (PlayerForm_Possess :type Actor%20Object%20Reference))
  (bind _output_get (Variables|PlayerForms|SetCurrentPF CurrentPlayerForm))
  (bind (_pc_sky _pf_island _pf_normal _pf_spirit _pf_dead) (Class|BPIPlayerForm|GetPlayerForm(Message) PlayerForm_Possess))
  (switch Utilities|FlowControl|Switch|SwitchonEPlayerForm _output_get
    (:Island
      (Variables|PlayerForms|SetPF_Island _pf_island))
    (:Normal
      (Variables|PlayerForms|SetPF_Normal _pf_normal))
    (:Spirit
      (Variables|PlayerForms|SetPF_Spirit _pf_spirit))
    (:Dead
      (Variables|PlayerForms|SetPF_Dead _pf_dead))))

(event Custom|Multicast_StoredQSI
  (params (StoredQSI :type Integer))
  (Variables|Default|SetStoredQSI StoredQSI))

(event Custom|TypingChat
  (bind _pf_normal (Variables|PlayerForms|GetPF_Normal))
  (bind _w_pf_normal (Variables|/Game/Blueprints/PF_Normal.PF_Normal_C|GetW_PF_Normal _pf_normal))
  ;[1 1 1] Chat
  (Input|SetInputModeGameandUI (Variables|Default|GetBP_PlayerController) (Variables|/Game/Widgets/W_PF_Normal.W_PF_Normal_C|GetMessageInput (Variables|/Game/Blueprints/PF_Normal.PF_Normal_C|GetW_PF_Normal (Variables|PlayerForms|GetPF_Normal))) "DoNotLock" true)
  (Variables|/Script/Engine.PlayerController|SetbShowMouseCursor (Variables|Default|GetBP_PlayerController) true)
  (Class|UserWidget|StopAnimation _w_pf_normal (Variables|/Game/Widgets/W_PF_Normal.W_PF_Normal_C|GetHideChat _w_pf_normal))
  (Widget|SetRenderOpacity (Variables|/Game/Widgets/W_PF_Normal.W_PF_Normal_C|GetChat _w_pf_normal) 1.0))

(event Custom|Server_SetPawnIslandControl
  (params (Pawn :type Pawn%20Object%20Reference))
  (bind _islandarchon (Variables|Default|GetIslandArchon))
  (bind _pawn_island_control (Variables|/Game/Blueprints/IslandArchon.IslandArchon_C|GetPawn%20Island%20Control _islandarchon))
  (Default|MulticastPossessControlPawn _pawn_island_control Pawn self)
  (Game|Player|SetViewTargetwithBlend (Variables|Default|GetBP_PlayerController) _pawn_island_control 1.0 "VTBlend_EaseInOut" 2.0 false)
  (Default|PossessPawn (Variables|Default|GetBP_PlayerController) _pawn_island_control true))

(event EventBeginPlay
  (CallFunction|EnsureInit)
  (Utilities|IsOwner
    (:OwningClient
      (Default|ClientStartPlayer (Variables|Default|GetBP_PlayerController)))))

(event Input|ActionEvents|InputActionChat
  (params (Key :type Key%20Structure :default "None"))
  ;[1 1 1] Chat
  (:Pressed
    (CallFunction|TypingChat)))

(fn ConstructionScript)

(fn SetMousetoCenter
  (bind _returnvalue (Viewport|GetViewportSize))
  (Class|PlayerController|SetMouseLocation (Variables|Default|GetBP_PlayerController) (Math|Float|Truncate (/ (.x _returnvalue) 2.0)) (Math|Float|Truncate (/ (.y _returnvalue) 2.0))))

(fn GetPlayerForm
  (return (Variables|Default|GetBP_PlayerController) (Variables|PlayerForms|GetPF_Island) (Variables|PlayerForms|GetPF_Normal) (Variables|PlayerForms|GetPF_Spirit) (Variables|PlayerForms|GetPF_Dead)))