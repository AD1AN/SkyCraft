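; BP_IslandArchon is a moving sky island that players can crystallize, resize and control through crystal or non-crystal menus.
; The server spawns its CrystalArchon and control pawn, restores or randomizes heading, and halts it on island collision.
; Tick interpolates direction and speed and teleports the actor to keep attached physics stable.
; Essence pays for crystallizing and expansion, deficit drops speed, and RepNotifies and multicasts drive UI events and rumble effects.
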(event OnComponentBeginOverlap(IslandCollision)
  (params (OverlappedComponent :type Primitive%20Component%20Object%20Reference) (OtherActor :type Actor%20Object%20Reference) (OtherComp :type Primitive%20Component%20Object%20Reference) (OtherBodyIndex :type Integer) (bFromSweep :type Boolean) (SweepResult :type Hit%20Result%20Structure%20%28by%20ref%29))
  (Utilities|IsValid OtherActor
    (:Is%20Valid
      (if (and (!= OtherActor self) (Class|GameplayStatics|ObjectIsA OtherActor "/Script/SkyCraft.Island"))
        (CallFunction|MulticastFXIslandCollide)
        (CallFunction|ServerStopIsland)))))

(event Custom|StartResizeIsland
  (params (NewSize :type Integer) (PlayerInstigator :type BP%20PSS%20Object%20Reference))
  (bind _sizenum (CallFunction|GetIslandSizeNum))
  (bind _sizenum_2 (CallFunction|GetIslandSizeNum))
  (bind _shrinkcost (Variables|ConfigVariables|GetShrinkCost))
  (bind _expandcost (Variables|ConfigVariables|GetExpandCost))
  (bind _returnvalue (- _sizenum_2 NewSize))
  (bind _returnvalue_2 (- NewSize _sizenum))
  (bind _returnvalue_3 (* _returnvalue_2 _expandcost))
  (bind _returnvalue_4 (* _returnvalue _shrinkcost))
  (bind _returnvalue_5 (/ _returnvalue_4 3))
  (if (and (!= NewSize (CallFunction|GetIslandSizeNum)) (not (Variables|Default|GetResizing)))
    (if (> NewSize (CallFunction|GetIslandSizeNum))
      (if (CallFunction|CheckEnoughEssence _returnvalue_3)
        (bind _valid (CallFunction|CheckResizeSpace NewSize))
        (if _valid
          (bind _returnvalue_6 (Class|AdianFL|UniformSubtract (Variables|Default|GetEssence) _returnvalue_3))
          (Variables|Default|SetEssence (.finalessence _returnvalue_6))
          (Variables|Default|SetResizeNewSize NewSize :!label _label)
          (CallFunction|ServerStopIsland)
          (Variables|Default|SetResizing true)
          (CallFunction|MulticastFXStartResize)
          (Utilities|Time|SetTimerbyEvent (delegate Custom|FinishResize) 5.0)
          (else
            (Default|ClientShowWarning PlayerInstigator "Another island is blocking your island's expansion."))))
      (else
        (Variables|Default|SetEssence (Class|AdianFL|AddEssence (Utilities|Struct|MakeEssence _returnvalue_5 _returnvalue_5 _returnvalue_5) (Variables|Default|GetEssence)))
        (goto _label)))))

(event Custom|FinishResize
  (Class|IslandArchon|SetIslandSize (* (Math|Conversions|ToFloat(Integer) (Variables|Default|GetResizeNewSize)) 0.01))
  (Variables|Default|SetResizing false)
  (CallFunction|MulticastFXCompleteResize))

(event Custom|Server_StopIsland
  (CallFunction|MulticastStopIsland (Variables|IslandMovement|GetPreviousLocation)))

(event Custom|MulticastFX_IslandCollide
  (Audio|SpawnSoundAttached "/Game/Audio/SFX/IslandCollide.IslandCollide" (Variables|Transformation|GetRootComponent) "None" "0, 0, 0" "0, 0, 0" "KeepRelativeOffset" false (Math|Float|MapRangeClamped (Variables|IslandMovement|GetCurrentSpeed) 0.0 (/ (Variables|ConfigVariables|GetTargetSpeedMax) 2.5) 0.05 1.0) 1.0 0.0 "/Game/Audio/WholeIslandAttenuation.WholeIslandAttenuation" 0)
  (Camera|PlayWorldCameraShake "/Game/Blueprints/CameraShake/CS_IslandCollide.CS_IslandCollide_C" (Transformation|GetActorLocation) 1e+04 5e+03))

(event Custom|MulticastFX_CompleteResize
  (bind _shaperadius (Variables|Default|GetShapeRadius))
  (bind _cs_rumble (Variables|Default|GetCS_Rumble))
  (bind _ns_islandrumble (Variables|Default|GetNS_IslandRumble))
  (bind _returnvalue (+ _shaperadius 8e+03))
  (if (not (Networking|IsDedicatedServer))
    (Class|AudioParameterControllerInterface|SetTriggerParameter (Variables|Default|GetAudioRumble) "CompleteResize")
    (Camera|PlayWorldCameraShake "/Game/Blueprints/CameraShake/CS_BigImpact.CS_BigImpact_C" (Transformation|GetActorLocation) _returnvalue _returnvalue)
    (Utilities|FlowControl|Sequence
      (:then_0
        (Utilities|IsValid _cs_rumble
          (:Is%20Valid
            (CameraShake|StopAllCameraShakes _cs_rumble false)
            (Components|DestroyComponent (Variables|Default|GetCS_Rumble)))))
      (:then_1
        (Utilities|IsValid _ns_islandrumble
          (:Is%20Valid
            (Components|Activation|SetActive _ns_islandrumble false false)))))))

(event Custom|MulticastFX_StartResize
  (if (not (Networking|IsDedicatedServer))
    (Audio|Components|Audio|Play (Variables|Default|GetAudioRumble) 0.0)
    (bind _returnvalue (AddComponent|AddCameraShakeSourceComponent false))
    (bind _output_get (Variables|Default|SetCS_Rumble _returnvalue))
    (bind _output_get_2 (Variables|/Script/Engine.CameraShakeSourceComponent|SetInnerAttenuationRadius _output_get (+ (Variables|Default|GetShapeRadius) 8e+03)))
    (Variables|/Script/Engine.CameraShakeSourceComponent|SetOuterAttenuationRadius _output_get _output_get_2)
    (bind _returnvalue_2 (Niagara|SpawnSystemAttached "/Game/Niagara/NS_IslandRumble.NS_IslandRumble" (Variables|Transformation|GetRootComponent) "None" "0, 0, 0" "0, 0, 0" "KeepRelativeOffset" true))
    (bind _output_get_3 (Variables|Default|SetNS_IslandRumble _returnvalue_2))
    (Class|NiagaraDataInterfaceArrayFunctionLibrary|SetNiagaraArrayPosition _output_get_3 "Vertices" (.topvertices (Variables|Default|GetID)))
    (Niagara|SetNiagaraVariable(Float) _output_get_3 "IslandSizeRatio" (Variables|Default|GetIslandSize))))

(event Custom|Multicast_StopIsland
  (params (ServerLocation :type Vector%20Net%20Quantize%2010%20Structure))
  (Transformation|SetActorLocation ServerLocation false true)
  (Variables|IslandMovement|SetStopIsland true)
  (Variables|IslandMovement|SetCurrentSpeed 0.0)
  (Variables|IslandMovement|SetAltitudeDirection 0.0)
  (Variables|IslandMovement|SetTargetAltitude (.z (Variables|IslandMovement|GetPreviousLocation)))
  (Audio|SpawnSoundAttached "/Game/Audio/SFX/IslandStop.IslandStop" (Variables|Transformation|GetRootComponent) "None" "0, 0, 0" "0, 0, 0" "KeepRelativeOffset" false 1.0 1.0 0.0 "/Game/Audio/WholeIslandAttenuation.WholeIslandAttenuation" 0))

(event Custom|OnEssenceChange_Event
  (CallFunction|CheckEssenceDeficit))

(event Custom|OnDie_Event
  (Class|IslandArchon|AuthSetCrystal false))

(event Custom|OnIslandSize_Event
  (bind _shaperadius (Variables|Default|GetShapeRadius))
  (Components|Capsule|SetCapsuleRadius (Variables|Default|GetIslandCollision) (Variables|Default|GetShapeRadius) true)
  (Components|Capsule|SetCapsuleHalfHeight (Variables|Default|GetIslandCollision) (* 1.25 _shaperadius) true)
  (Transformation|SetRelativeLocation (Variables|Default|GetIslandCollision) (Math|Vector|MakeVector 0.0 0.0 (* -0.2 _shaperadius)) false true)
  (Niagara|SetNiagaraVariable(Float) (Variables|Default|GetNS_Outside) "Radius" (+ 1e+03 (Variables|Default|GetShapeRadius)))
  (Niagara|SetNiagaraVariable(Float) (Variables|Default|GetNS_Wind) "Radius" (Variables|Default|GetShapeRadius))
  (Niagara|SetNiagaraVariable(Float) (Variables|Default|GetNS_Wind) "IslandSizeRatio" (Variables|Default|GetIslandSize))
  (Utilities|Struct|SetmembersinSoundAttenuationSettings (Variables|/Script/Engine.AudioComponent|GetAttenuationOverrides (Variables|Default|GetAudioRumble)) (Math|Vector|MakeVector (+ (Variables|Default|GetShapeRadius) 5e+03) 0.0 0.0)))

(event Custom|Multicast_UnstopIsland
  (Variables|IslandMovement|SetStopIsland false))

(event Custom|Server_UnstopIsland
  (if (> (Class|AdianFL|EssenceTotal (Variables|Default|GetEssence)) 0)
    (CallFunction|MulticastUnstopIsland)))

(event EventBeginPlay
  (bind _ss_islandarchon (Variables|Default|GetSS_IslandArchon))
  (bind (_islandsize _archonsteamid _targetdirection _targetaltitude _targetspeed _stopisland _essence _astralons) (Utilities|Struct|BreakSS_IslandArchon _ss_islandarchon))
  (Utilities|FlowControl|Sequence
    (:then_0
      (Networking|SwitchHasAuthority
        (:Authority
          (Collision|SetCollisionEnabled (Variables|Default|GetIslandCollision) "QueryOnly")
          (bind _returnvalue (Game|SpawnActorfromClass "/Game/Blueprints/CrystalArchon.CrystalArchon_C" (Math|Transform|MakeTransform "0, 0, 0" "0, 0, 0" "1.000000,1.000000,1.000000") "AlwaysSpawn" "MultiplyWithRoot" 0 self 0))
          (Variables|Default|SetCrystalArchon _returnvalue)
          (bind _returnvalue_2 (Game|SpawnActorfromClass "/Game/Blueprints/Pawn_IslandControl.Pawn_IslandControl_C" (Math|Transform|MakeTransform "0, 0, 0" "0, 0, 0" "1.000000,1.000000,1.000000") "AlwaysSpawn" "MultiplyWithRoot" 0 self 0))
          (bind _output_get (Variables|Default|SetPawn%20Island%20Control _returnvalue_2))
          (Transformation|AttachActorToActor _output_get self "None" "KeepRelative" "KeepRelative" "KeepRelative" false)
          (bind _asbp_gms (Utilities|Casting|CastToBP_GMS (Game|GetGameMode)))
          (Variables|LocalVariables|SetBP_GMS _asbp_gms)
          (EventDispatchers|BindEventtoOnDie (Variables|/Game/Blueprints/CrystalArchon.CrystalArchon_C|GetHealthSystem (Variables|Default|GetCrystalArchon)) (delegate Custom|OnDie_Event))
          (EventDispatchers|AssignOnEssence (delegate Custom|OnEssenceChange_Event))
          (Variables|IslandMovement|SetTargetAltitude (.z (Transformation|GetActorLocation)))
          (if (Variables|Default|GetbLoadFromSave)
            (Class|IslandArchon|AuthSetArchonSteamID _archonsteamid)
            (Variables|IslandMovement|SetTargetDirection _targetdirection)
            (Variables|IslandMovement|SetTargetAltitude _targetaltitude)
            (Variables|IslandMovement|SetTargetSpeed _targetspeed)
            (Variables|IslandMovement|SetStopIsland _stopisland)
            (Variables|Default|SetEssence _essence)
            (Variables|Default|SetSS_Astralons _astralons)
            (else
              (bind _output_get_2 (Variables|IslandMovement|SetTargetDirection (Math|Vector|GetForwardVector (Math|Rotator|MakeRotator 0.0 0.0 (.yaw (Math|Random|RandomRotator false))))))
              (Variables|IslandMovement|SetCurrentDirection _output_get_2)
              (bind _output_get_3 (Variables|IslandMovement|SetTargetSpeed (Variables|ConfigVariables|GetTargetSpeedMin)))
              (Variables|IslandMovement|SetCurrentSpeed _output_get_3))))))
    (:then_1
      (EventDispatchers|AssignOnIslandSize (delegate Custom|OnIslandSize_Event))
      (CallFunction|OnIslandSizeEvent)
      (Variables|Default|SetIslandStarted true))))

(event EventTick
  (params (DeltaSeconds :type Float%20%28single-precision%29))
  (bind _returnvalue (Transformation|GetActorLocation))
  (bind _returnvalue_2 (Transformation|GetActorLocation))
  (bind _returnvalue_3 (Transformation|GetActorLocation))
  (bind _targetaltitude (Variables|IslandMovement|GetTargetAltitude))
  (Variables|IslandMovement|SetPreviousLocation (Math|Vector|MakeVectorNetQuantize10 (.x _returnvalue_3) (.y _returnvalue_3) (.z _returnvalue_3)))
  (Transformation|SetActorLocation (+ (* (Math|Vector|MakeVector (.x (* (Variables|IslandMovement|GetCurrentDirection) (Variables|IslandMovement|GetCurrentSpeed))) (.y (* (Variables|IslandMovement|GetCurrentDirection) (Variables|IslandMovement|GetCurrentSpeed))) (+ (* (Variables|IslandMovement|GetAltitudeDirection) 5.0) (* (Variables|IslandMovement|GetAltitudeDirection) (Variables|IslandMovement|GetCurrentSpeed) 0.01))) (Utilities|Time|GetWorldDeltaSeconds)) (Transformation|GetActorLocation)) false true) ; Should be Teleport = true\nOtherwise attached physics objects\nwill fly away.
  (Variables|IslandMovement|SetCurrentDirection (Math|Interpolation|VInterpTo (Variables|IslandMovement|GetCurrentDirection) (Variables|IslandMovement|GetTargetDirection) (Utilities|Time|GetWorldDeltaSeconds) 1.0))
  (Variables|IslandMovement|SetCurrentSpeed (Math|Interpolation|FInterpTo (Variables|IslandMovement|GetCurrentSpeed) (select (Variables|IslandMovement|GetStopIsland) 0.0 (Variables|IslandMovement|GetTargetSpeed)) (Utilities|Time|GetWorldDeltaSeconds) 0.75))
  (if (!= (Variables|IslandMovement|GetAltitudeDirection) 0.0) ; If Altitude != 0
    (if (select (> (Variables|IslandMovement|GetAltitudeDirection) 0.0) (>= (.z _returnvalue_2) _targetaltitude) (<= (.z _returnvalue_2) _targetaltitude))
      (Variables|IslandMovement|SetAltitudeDirection 0.0)
      (Transformation|SetActorLocation (Math|Vector|MakeVector (.x _returnvalue) (.y _returnvalue) (Variables|IslandMovement|GetTargetAltitude)) false true))))

(event EventOnIslandShrink
  (for _array_element (Variables|Default|GetBuildings)
    (if (Class|AdianFL|ActorHasSkyTag _array_element "/Game/DataAssets/SkyTag/Building_Foundation.Building_Foundation")
      (bind _asbm_foundation (Utilities|Casting|CastToBM_Foundation _array_element))
      (bind _valid (Default|GridTraces _asbm_foundation))
      (if (not _valid)
        (Class|BM|Dismantle _asbm_foundation)))))

(event EventOnRepCrystal
  (bind _returnvalue (Transformation|GetActorLocation))
  (bind _returnvalue_2 (Transformation|GetActorLocation))
  (bind _shaperadius (Variables|Default|GetShapeRadius))
  (bind _shaperadius_2 (Variables|Default|GetShapeRadius))
  (bind _buildings (Variables|Default|GetBuildings))
  (bind _returnvalue_3 (+ _shaperadius_2 8e+03))
  (bind _returnvalue_4 (+ _shaperadius 8e+03))
  (if (Variables|Default|GetIslandStarted)
    (|CallParentFunction)
    (Utilities|FlowControl|Sequence
      (:then_0
        (if (Variables|Default|GetCrystal)
          (Variables|Default|SetbIslandCanSave true)
          (if (not (Networking|IsDedicatedServer))
            (bind _returnvalue_5 (Niagara|SpawnSystemAttached "/Game/Niagara/NS_IslandGroundBurst.NS_IslandGroundBurst" (Variables|Transformation|GetRootComponent) "None" "0, 0, 0" "0, 0, 0" "KeepRelativeOffset" true))
            (Class|NiagaraDataInterfaceArrayFunctionLibrary|SetNiagaraArrayPosition _returnvalue_5 "Vertices" (.topvertices (Variables|Default|GetID)))
            (Niagara|SetNiagaraVariable(Float) _returnvalue_5 "IslandSizeRatio" (Variables|Default|GetIslandSize))
            (Audio|SpawnSoundatLocation "/Game/Audio/SFX/Death.Death" _returnvalue "0, 0, 0" 3.0 0.75 0.0 "/Game/Audio/WholeIslandAttenuation.WholeIslandAttenuation" 0)
            (Audio|SpawnSoundatLocation "/Game/Audio/SFX/IslandRumbleCompleteResize.IslandRumbleCompleteResize" _returnvalue "0, 0, 0" 2.0 0.8 0.0 "/Game/Audio/WholeIslandAttenuation.WholeIslandAttenuation" 0)
            (Camera|PlayWorldCameraShake "/Game/Blueprints/CameraShake/CS_BigImpact.CS_BigImpact_C" (Transformation|GetActorLocation) _returnvalue_3 _returnvalue_3))
          (else
            (Actor|DestroyActor _buildings)
            (Utilities|Array|Clear _buildings)
            (Audio|SpawnSoundatLocation "/Game/Audio/SFX/Death.Death" _returnvalue_2 "0, 0, 0" 3.0 0.75 0.0 "/Game/Audio/WholeIslandAttenuation.WholeIslandAttenuation" 0)
            (Audio|SpawnSoundatLocation "/Game/Audio/SFX/IslandRumbleCompleteResize.IslandRumbleCompleteResize" _returnvalue_2 "0, 0, 0" 2.0 0.8 0.0 "/Game/Audio/WholeIslandAttenuation.WholeIslandAttenuation" 0)
            (Camera|PlayWorldCameraShake "/Game/Blueprints/CameraShake/CS_BigImpact.CS_BigImpact_C" (Transformation|GetActorLocation) _returnvalue_4 _returnvalue_4)
            (Networking|SwitchHasAuthority
              (:Authority
                (CallFunction|ServerStopIsland))))))
      (:then_1
        (Networking|SwitchHasAuthority
          (:Authority
            (Variables|Default|SetEssenceDeficit false)))))))

(fn ConstructionScript)

(fn OnRepStopIsland
  (Default|CallOnStopIsland))

(fn OnRepTargetDirection
  (Default|CallOnTargetDirection)
  (Niagara|SetNiagaraVariable(Float) (Variables|Default|GetNS_Wind) "YawDirection" (- (.yaw (Math|Conversions|RotationFromXVector (Variables|IslandMovement|GetTargetDirection))) 9e+01)))

(fn OnRepEssence
  (Default|CallOnEssence))

(fn OnRepTargetSpeed
  (bind _output_get (Variables|IslandMovement|SetTargetSpeedRatio (Math|Float|MapRangeClamped (Variables|IslandMovement|GetTargetSpeed) (Variables|ConfigVariables|GetTargetSpeedMin) (Variables|ConfigVariables|GetTargetSpeedMax) 0.0 1.0)))
  (Niagara|SetNiagaraVariable(Float) (Variables|Default|GetNS_Wind) "TargetSpeedRatio" _output_get)
  (Default|CallOnTargetSpeed))

(fn CreateMenu
  (params (Pawn :type Pawn%20Object%20Reference) (BP_PSS :type BP%20PSS%20Object%20Reference))
  (if (Variables|Default|GetCrystal)
    (Utilities|IsValid (Variables|LocalVariables|GetCWS_Crystal_IslandArchon)
      (:Is%20Valid
        _)
      (:Is%20Not%20Valid
        (bind _returnvalue (UserInterface|CreateWidget "/Game/Widgets/CWS/CWS_Crystal_IslandArchon.CWS_Crystal_IslandArchon_C" 0 self))
        (Variables|LocalVariables|SetCWS_Crystal_IslandArchon _returnvalue)))
    (Default|ShowMenu (Variables|LocalVariables|GetCWS_Crystal_IslandArchon) (EventDispatchers|CreateEvent :!event ShowCompleted))
    (UserInterface|Viewport|AddtoViewport (Variables|LocalVariables|GetCWS_Crystal_IslandArchon) 20)
    (Default|AddCWS BP_PSS (Variables|LocalVariables|GetCWS_Crystal_IslandArchon) true true true "NewEnumerator2")
    (Default|SetMouseto BP_PSS 2.0 2.0)
    (else
      (Utilities|IsValid (Variables|LocalVariables|GetCWS_NonCrystal_IslandArchon)
        (:Is%20Valid
          _)
        (:Is%20Not%20Valid
          (bind _returnvalue_2 (UserInterface|CreateWidget "/Game/Widgets/CWS/CWS_NonCrystal_IslandArchon.CWS_NonCrystal_IslandArchon_C" 0 self))
          (Variables|LocalVariables|SetCWS_NonCrystal_IslandArchon _returnvalue_2)))
      (Default|ShowMenu (Variables|LocalVariables|GetCWS_NonCrystal_IslandArchon))
      (UserInterface|Viewport|AddtoViewport (Variables|LocalVariables|GetCWS_NonCrystal_IslandArchon) 20)
      (Default|AddCWS BP_PSS (Variables|LocalVariables|GetCWS_NonCrystal_IslandArchon) true true true "NewEnumerator2")
      (Default|SetMouseto BP_PSS 2.0 2.0))))

(fn ShowCompleted)

(fn CheckEnoughEssence
  (params (RequireEssence :type Integer))
  (return (> (Class|AdianFL|EssenceTotal (Variables|Default|GetEssence)) RequireEssence)))

(fn CheckEssenceDeficit
  (if (< (Class|AdianFL|EssenceTotal (Variables|Default|GetEssence)) 1000)
    (if (not (Variables|Default|GetEssenceDeficit))
      (Variables|Default|SetEssenceDeficit true)
      (Variables|IslandMovement|SetTargetSpeed (Variables|ConfigVariables|GetTargetSpeedMin))
      (Default|CallOnEssenceDeficit :!label _label))
    (elif (Variables|Default|GetEssenceDeficit)
      (Variables|Default|SetEssenceDeficit false)
      (goto _label))))

(fn OnRepBurnEssence
  (Default|CallOnBurnEssence))

(fn OnRepEssenceDeficit
  (Default|CallOnEssenceDeficit))

(fn OnRepCollapseTime
  (if (not (== (Variables|Default|GetCollapseTime) 0))
    (Default|CallOnCollapseTime)))

(fn OnRepCollapsing
  (Default|CallOnCollapsing)
  (Variables|Default|SetCollapseTime 0)
  (if (not (Networking|IsDedicatedServer))
    (if (Variables|Default|GetCollapsing)
      (Audio|Components|Audio|Play (Variables|Default|GetAudioRumble) 0.0)
      (Utilities|IsValid (Variables|Default|GetCS_Rumble)
        (:Is%20Valid
          (CameraShake|StopAllCameraShakes (Variables|Default|GetCS_Rumble) false)
          (Components|DestroyComponent (Variables|Default|GetCS_Rumble)))
        (:Is%20Not%20Valid
          _))
      (bind _returnvalue (AddComponent|AddCameraShakeSourceComponent false))
      (bind _output_get (Variables|Default|SetCS_Rumble _returnvalue))
      (bind _output_get_2 (Variables|/Script/Engine.CameraShakeSourceComponent|SetInnerAttenuationRadius _output_get (+ (Variables|Default|GetShapeRadius) 8e+03)))
      (Variables|/Script/Engine.CameraShakeSourceComponent|SetOuterAttenuationRadius _output_get _output_get_2)
      (Utilities|IsValid (Variables|Default|GetNS_IslandRumble)
        (:Is%20Valid
          (Class|AdianFL|ForceDestroyComponent (Variables|Default|GetNS_IslandRumble)))
        (:Is%20Not%20Valid
          _))
      (bind _returnvalue_2 (Niagara|SpawnSystemAttached "/Game/Niagara/NS_IslandRumble.NS_IslandRumble" (Variables|Transformation|GetRootComponent) "None" "0, 0, 0" "0, 0, 0" "KeepRelativeOffset" true))
      (bind _output_get_3 (Variables|Default|SetNS_IslandRumble _returnvalue_2))
      (Class|NiagaraDataInterfaceArrayFunctionLibrary|SetNiagaraArrayPosition _output_get_3 "Vertices" (.topvertices (Variables|Default|GetID)))
      (Niagara|SetNiagaraVariable(Float) _output_get_3 "IslandSizeRatio" (Variables|Default|GetIslandSize))
      (else
        (Class|AudioParameterControllerInterface|SetTriggerParameter (Variables|Default|GetAudioRumble) "RumbleStop")
        (Utilities|FlowControl|Sequence
          (:then_0
            (Utilities|IsValid (Variables|Default|GetCS_Rumble)
              (:Is%20Valid
                (CameraShake|StopAllCameraShakes (Variables|Default|GetCS_Rumble) false)
                (Components|DestroyComponent (Variables|Default|GetCS_Rumble)))))
          (:then_1
            (Utilities|IsValid (Variables|Default|GetNS_IslandRumble)
              (:Is%20Valid
                (Components|Activation|SetActive (Variables|Default|GetNS_IslandRumble) false false)))))))))

(fn Crystallize
  (if (>= (Class|AdianFL|EssenceTotal (Variables|Default|GetEssence)) (Variables|ConfigVariables|GetCrystallizeCost))
    (bind _returnvalue (Class|AdianFL|UniformSubtract (Variables|Default|GetEssence) (/ (Variables|ConfigVariables|GetCrystallizeCost) 2)))
    (Variables|Default|SetEssence (.finalessence _returnvalue))
    (Class|IslandArchon|AuthSetCrystal true)))

(fn CheckResizeSpace
  (params (NewSize :type Integer))
  (bind _returnvalue (Transformation|GetActorLocation))
  (bind _outhits (Collision|MultiSphereTraceByChannel _returnvalue _returnvalue (Math|Conversions|ToFloat(Integer) (+ (* NewSize 100) 1200)) "TraceTypeQuery1" false (Actor|GetAttachedActors true true) "None" true "(R=1.000000,G=0.000000,B=0.000000,A=1.000000)" "(R=0.000000,G=1.000000,B=0.000000,A=1.000000)" 1.0))
  (for _array_element _outhits
    (if (Class|GameplayStatics|ObjectIsA (.HitActor (Collision|BreakHitResult _array_element)) "/Script/SkyCraft.Island")
      (return false)))
  (return true))

(fn OnRepAltitudeDirection
  (Default|CallOnAltitudeDirection))

(fn OnRepTargetAltitude
  (Default|CallOnTargetAltitude))

(fn GetIslandSizeNum
  (return (Math|Float|Round (* (Variables|Default|GetIslandSize) 1e+02))))

(fn OnRepCrystalArchon
  (Default|CallOnRepCrystalArchon))

(fn AddEssence
  (params (AddEssence :type Essence%20Structure))
  (bind _output_get (Variables|Default|SetEssence (Class|AdianFL|AddEssence AddEssence (Variables|Default|GetEssence))))
  (return _output_get))

(fn GetEssence
  (return (Variables|Default|GetEssence)))

(fn SetEssence
  (params (NewEssence :type Essence%20Structure))
  (bind _output_get (Variables|Default|SetEssence NewEssence))
  (return _output_get))