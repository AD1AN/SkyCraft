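; Player-controlled flying island, procedurally generated, that steers, changes altitude and carries an essence-colored core.
; On the server it spawns an attached control pawn plus trees and stones.
; Tick eases direction and speed toward targets and multicasts them; overlapping another island stops it at its previous location.
; RepNotifies update core visuals and notify listeners, while interaction opens the island widget and attaches Spirit-form players.
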(event OnComponentBeginOverlap(PlayerIslandDetection)
  (params (OverlappedComponent :type Primitive%20Component%20Object%20Reference) (OtherActor :type Actor%20Object%20Reference) (OtherComp :type Primitive%20Component%20Object%20Reference) (OtherBodyIndex :type Integer) (bFromSweep :type Boolean) (SweepResult :type Hit%20Result%20Structure%20%28by%20ref%29))
  (if (Networking|IsServer)
    (Utilities|IsValid OtherActor
      (:Is%20Valid
        (if (Actor|ActorHasTag OtherActor "Island")
          (CallFunction|ServerStopPlayerIsland)
          (Variables|Default|SetCurrentDirection "0, 0, 0")
          (Transformation|SetActorLocation (Variables|Default|GetPreviousLocation) false false))))))

(event Custom|Server_StopPlayerIsland
  ;[1 1 1] Stop Island
  (Variables|Default|SetTargetDirection "0, 0, 0")
  (Variables|Default|SetCDT (Variables|Default|GetStop_CDT))
  (Variables|Default|SetAltitude 0.0)
  (Variables|Default|SetTargetAltitude (.z (Variables|Default|GetPreviousLocation)))
  (Variables|Default|SetStopIsland true))

(event Custom|Multicast_SetCurrentSpeed
  (params (CurrentSpeed :type Float%20%28double-precision%29))
  (Variables|Default|SetCurrentSpeed CurrentSpeed))

(event Custom|Multicast_SetCurrentDirection
  (params (CurrentDirection :type Vector))
  (Variables|Default|SetCurrentDirection CurrentDirection))

(event Custom|Multicast_PlayersInsideChange
  (params (PlayersInside :type Integer))
  (Variables|Default|SetPlayersInside PlayersInside)
  (Default|CallPlayersInsideChange))

(event EventBeginPlay
  (bind _boxresourcespawner (Variables|Default|GetBoxResourceSpawner))
  (bind _generator (Variables|Default|GetGenerator))
  (bind _boxresourcespawner_2 (Variables|Default|GetBoxResourceSpawner))
  (Utilities|FlowControl|Sequence
    (:then_0
      (if (not (Class|VoxelWorld|IsCreated))
        (Class|VoxelGeneratorTools|SetGeneratorParameter _generator "SeedName" (Class|KismetSystemLibrary|MakeLiteralInteger))
        (Class|VoxelGeneratorTools|SetGeneratorParameter _generator "Scale" (Math|Random|RandomIntegerinRangefromStream 20 20 (Math|Random|MakeRandomStream 0)))
        (Class|VoxelWorld|CreateWorld)))
    (:then_1
      (if (Networking|IsServer)
        (Variables|Default|SetTargetAltitude (.z (Transformation|GetActorLocation)))
        (bind _returnvalue (Game|SpawnActorfromClass "/Game/Blueprints/Pawn_IslandControl.Pawn_IslandControl_C" (Math|Transform|MakeTransform "0, 0, 0" "0, 0, 0" "1.000000,1.000000,1.000000") "AlwaysSpawn" 0 self 0))
        (bind _output_get (Variables|Default|SetPawn%20Island%20Control _returnvalue))
        (Transformation|AttachActorToActor _output_get self "None" "KeepRelative" "KeepRelative" "KeepRelative" true)
        (bind _gm_sky (Class|BPIGameMS|GetGMSky(Message) (Game|GetGameMode)))
        (Variables|Default|SetGM_Sky _gm_sky)
        (if (Variables|/Game/Blueprints/GM_Sky.GM_Sky_C|GetPlayerIslandLoadedFromSave (Variables|Default|GetGM_Sky))
          _
          (else
            (bind _output_get_2 (Variables|Default|SetTargetDirection (Math|Vector|GetForwardVector (Math|Rotator|MakeRotator 0.0 0.0 (.yaw (Math|Random|RandomRotator false))))))
            (Variables|Default|SetCurrentDirection _output_get_2)))
        (Utilities|FlowControl|Sequence
          (:then_0
            (for _index (range 0 4)
              (bind _returnvalue_2 (Game|SpawnActorfromClass "/Game/Blueprints/A_Tree.A_Tree_C" (Math|Transform|MakeTransform (Math|Random|RandomPointinBoundingBox (Transformation|GetWorldLocation _boxresourcespawner_2) (Components|Box|GetScaledBoxExtent _boxresourcespawner_2)) "0, 0, 0" "1.000000,1.000000,1.000000") "AlwaysSpawn" 0 0))
              (Transformation|AttachActorToActor _returnvalue_2 self "None" "KeepWorld" "KeepWorld" "KeepWorld" true)))
          (:then_1
            (for _index_2 (range 0 4)
              (bind _returnvalue_3 (Game|SpawnActorfromClass "/Game/Blueprints/A_Stone.A_Stone_C" (Math|Transform|MakeTransform (+ (Math|Random|RandomPointinBoundingBox (Transformation|GetWorldLocation _boxresourcespawner) (Components|Box|GetScaledBoxExtent _boxresourcespawner)) "0,0,40.000000") "0, 0, 0" "1.000000,1.000000,1.000000") "AlwaysSpawn" 0 0))
              (Transformation|AttachActorToActor _returnvalue_3 self "None" "KeepWorld" "KeepWorld" "KeepWorld" true))))))))

(event EventTick
  (params (DeltaSeconds :type Float%20%28single-precision%29))
  (bind _returnvalue (Transformation|GetActorLocation))
  (bind _returnvalue_2 (Transformation|GetActorLocation))
  (bind _returnvalue_3 (Transformation|GetActorLocation))
  (Utilities|FlowControl|Sequence
    (:then_0
      (if (not (Variables|Default|GetStopIsland))
        (Variables|Default|SetPreviousLocation (Transformation|GetActorLocation))))
    (:then_1
      (Transformation|SetActorLocation (+ (Math|Vector|MakeVector (.x (* (Variables|Default|GetCurrentDirection) (Variables|Default|GetCurrentSpeed))) (.y (* (Variables|Default|GetCurrentDirection) (Variables|Default|GetCurrentSpeed))) (* (Variables|Default|GetAltitude) (* (Variables|Default|GetCurrentSpeed) 0.05))) (Transformation|GetActorLocation)) false false)
      (bind _output_get (Variables|Default|SetCurrentDirection (Math|Interpolation|VInterpTo (Variables|Default|GetCurrentDirection) (Variables|Default|GetTargetDirection) (Utilities|Time|GetWorldDeltaSeconds) (Variables|Default|GetCDT))))
      (CallFunction|MulticastSetCurrentDirection _output_get)
      (bind _output_get_2 (Variables|Default|SetCurrentSpeed (Math|Interpolation|FInterpTo (Variables|Default|GetCurrentSpeed) (Variables|Default|GetTargetSpeed) (Utilities|Time|GetWorldDeltaSeconds) 0.5)))
      (CallFunction|MulticastSetCurrentSpeed _output_get_2)
      (if (!= (Variables|Default|GetAltitude) 0.0) ; If Altitude != 0
        (if (Math|Float|NearlyEqual(Float) (Variables|Default|GetTargetAltitude) (.z (Transformation|GetActorLocation)) (* (Variables|Default|GetCurrentSpeed) 5e+01 (Utilities|Time|GetWorldDeltaSeconds))) ; Near Target Altitude
          (Variables|Default|SetAltitude 0.0)
          (Transformation|SetActorLocation (Math|Vector|MakeVector (.x _returnvalue_2) (.y _returnvalue_2) (Variables|Default|GetTargetAltitude)) false false)
          (elif (> 0.0 (Variables|Default|GetAltitude)) ; For safety
            (if (< (.z (Transformation|GetActorLocation)) (Variables|Default|GetTargetAltitude))
              (Variables|Default|SetAltitude 0.0)
              (Transformation|SetActorLocation (Math|Vector|MakeVector (.x _returnvalue_3) (.y _returnvalue_3) (Variables|Default|GetTargetAltitude)) false false))
            (elif (> (.z (Transformation|GetActorLocation)) (Variables|Default|GetTargetAltitude))
              (Variables|Default|SetAltitude 0.0)
              (Transformation|SetActorLocation (Math|Vector|MakeVector (.x _returnvalue) (.y _returnvalue) (Variables|Default|GetTargetAltitude)) false false))))))))

(fn ConstructionScript
  (bind _generator (Variables|Default|GetGenerator))
  (if (not (Class|VoxelWorld|IsCreated))
    (Class|VoxelGeneratorTools|SetGeneratorParameter _generator "SeedName" (Class|KismetSystemLibrary|MakeLiteralInteger))
    (Class|VoxelGeneratorTools|SetGeneratorParameter _generator "Scale" (Math|Random|RandomIntegerinRangefromStream 20 20 (Math|Random|MakeRandomStream 0)))
    (Class|VoxelWorld|CreateWorld)))

(fn OnRepStopIsland
  (Default|CallStopIslandChange))

(fn OnRepTargetDirection
  (Niagara|SetNiagaraVariable(Vector3) (Variables|Default|GetNiagara_PlayerIslandCore) "AttractorPosition" (* (Variables|Default|GetTargetDirection) 1e+02)))

(fn OnRepEssence
  (bind _essence (Variables|Default|GetEssence))
  (bind (_r _g _b) (CallFunction|EssenceRGB _essence))
  (Default|CallPlayerIslandEssenceChange)
  (Niagara|SetNiagaraVariable(LinearColor) (Variables|Default|GetNiagara_PlayerIslandCore) "EssenceColor" (Utilities|Struct|MakeLinearColor _r _g _b 1.0))
  (CallFunction|UpdateCoreColor))

(fn OnRepTargetSpeed
  (Default|CallTargetSpeedChange))

(fn OnRepEssenceBurnSelect
  (Default|CallEssenceBurnSelectChange))

(fn UpdateCoreColor
  (bind _essence (Variables|Default|GetEssence))
  (bind (_r _g _b) (CallFunction|EssenceRGB _essence))
  (Rendering|Material|SetVectorParameterValueonMaterials (Variables|Default|GetIslandCore) "EssenceColor" (Math|Vector|MakeVector _r _g _b)))

(fn ConsumeEssence
  (params (Essence :type S%20Essence%20Structure))
  (Variables|Default|SetEssence (CallFunction|AddEssence (Utilities|Struct|MakeS_Essence (/ (.red Essence) 2) (/ (.green Essence) 2) (/ (.blue Essence) 2)) (Variables|Default|GetEssence)))
  (return true))

(fn GetACInteract
  (return (Variables|Default|GetAC_Interact)))

(fn GetEssence
  (return ""))

(fn GetInteractionLocation
  (return (Transformation|GetWorldLocation (Variables|Default|GetIslandCore))))

(fn GetPlayerIsland
  (return self))

(fn INT1Client
  (params (InteractedPawn :type Pawn%20Object%20Reference) (InteractedPC_Sky :type PC%20Sky%20Object%20Reference) (InteractedWith :type IC%20Class%20Reference))
  (bind _returnvalue (UserInterface|CreateWidget "/Game/Widgets/CWS/CWS_PlayerIsland.CWS_PlayerIsland_C" InteractedPC_Sky self InteractedPC_Sky InteractedPawn)) ; One more in Pawn_IslandControl(Interact)
  (UserInterface|Viewport|AddtoViewport _returnvalue 0)
  (Default|AddCWS InteractedPC_Sky _returnvalue)
  (Default|SetMousetoCenter InteractedPC_Sky)
  (return true))

(fn INT1ClientInterrupt
  (params (InteractedPawn :type Pawn%20Object%20Reference) (InteractedPC_Sky :type PC%20Sky%20Object%20Reference) (InteractedWith :type IC%20Class%20Reference))
  (return false))

(fn INT1Server
  (params (InteractedPawn :type Pawn%20Object%20Reference) (InteractedPC_Sky :type PC%20Sky%20Object%20Reference) (InteractedWith :type IC%20Class%20Reference))
  (switch Utilities|FlowControl|Switch|SwitchonE_CurrentPlayerForm (Variables|/Game/Blueprints/PC_Sky.PC_Sky_C|GetCurrentPlayerForm InteractedPC_Sky)
    (:NewEnumerator2
      (return false))
    (:NewEnumerator3
      (Transformation|AttachActorToActor InteractedPawn self "None" "KeepWorld" "KeepWorld" "KeepWorld" true)
      (return true))))

(fn INT1ServerInterrupt
  (params (InteractedPawn :type Pawn%20Object%20Reference) (InteractedPC_Sky :type PC%20Sky%20Object%20Reference) (InteractedWith :type IC%20Class%20Reference))
  (switch Utilities|FlowControl|Switch|SwitchonE_CurrentPlayerForm (Variables|/Game/Blueprints/PC_Sky.PC_Sky_C|GetCurrentPlayerForm InteractedPC_Sky)
    (:NewEnumerator2
      (return false))
    (:NewEnumerator3
      (Transformation|DetachFromActor InteractedPawn "KeepWorld" "KeepWorld" "KeepWorld")
      (return true))))

(fn INT2Client
  (params (InteractedPawn :type Pawn%20Object%20Reference) (InteractedPC_Sky :type PC%20Sky%20Object%20Reference) (InteractedWith :type IC%20Class%20Reference))
  (return false))

(fn INT2ClientInterrupt
  (params (InteractedPawn :type Pawn%20Object%20Reference) (InteractedPC_Sky :type PC%20Sky%20Object%20Reference) (InteractedWith :type IC%20Class%20Reference))
  (return false))

(fn INT2Server
  (params (InteractedPawn :type Pawn%20Object%20Reference) (InteractedPC_Sky :type PC%20Sky%20Object%20Reference) (InteractedWith :type IC%20Class%20Reference))
  (return false))

(fn INT2ServerInterrupt
  (params (InteractedPawn :type Pawn%20Object%20Reference) (InteractedPC_Sky :type PC%20Sky%20Object%20Reference) (InteractedWith :type IC%20Class%20Reference))
  (return false))

(fn INT3Client
  (params (InteractedPawn :type Pawn%20Object%20Reference) (InteractedPC_Sky :type PC%20Sky%20Object%20Reference) (InteractedWith :type IC%20Class%20Reference))
  (return false))

(fn INT3ClientInterrupt
  (params (InteractedPawn :type Pawn%20Object%20Reference) (InteractedPC_Sky :type PC%20Sky%20Object%20Reference) (InteractedWith :type IC%20Class%20Reference))
  (return false))

(fn INT3Server
  (params (InteractedPawn :type Pawn%20Object%20Reference) (InteractedPC_Sky :type PC%20Sky%20Object%20Reference) (InteractedWith :type IC%20Class%20Reference))
  (return false))

(fn INT3ServerInterrupt
  (params (InteractedPawn :type Pawn%20Object%20Reference) (InteractedPC_Sky :type PC%20Sky%20Object%20Reference) (InteractedWith :type IC%20Class%20Reference))
  (return false))

(fn SetEssence(Server)
  (params (Essence :type S%20Essence%20Structure))
  (return ""))