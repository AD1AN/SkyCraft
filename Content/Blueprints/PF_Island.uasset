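; PF_Island is the player's island-form pawn, with an orbit camera, inventory and island menu, from which the player emerges as a PF_Normal character.
; Holding Jump fills a progress bar, then traces for ground ahead and asks the server to spawn that character with essence, inventory and equipment.
; A multicast spline timeline animates the spirit ball and fades blur, then the server transfers possession and destroys the island pawn.
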(event Custom|Server_SpawnNormal
  (params (SpawnTransform :type Transform))
  (CallFunction|SpawnPFNormal(Server) (.location SpawnTransform) (.rotation SpawnTransform)))

(event Custom|ShowCompleted)

(event Custom|HideCompleted
  (bind _w_pf_island (Variables|Default|GetW_PF_Island))
  (Utilities|IsValid _w_pf_island
    (:Is%20Valid
      (Widget|RemovefromParent _w_pf_island))))

(event Custom|Formed_Changed_Event_0
  (Transformation|SetRelativeLocation (Variables|Default|GetSkySpringArm) (Math|Vector|MakeVector 0.0 0.0 (Math|Float|SelectFloat 5e+01 0.0 (Variables|/Game/Blueprints/IslandArchon.IslandArchon_C|GetCrystal (Variables|/Game/Blueprints/BP_PAI.BP_PAI_C|GetIslandArchon (Variables|Default|GetBP_PAI))))) false false))

(event Custom|Client_Possessed
  (CallFunction|EnsureBeginPlay))

(event Custom|EnsureBeginPlay
  (if (not (Variables|Default|GethadBeginPlay))
    (Variables|Default|SethadBeginPlay true)
    (bind _asbp_sgi (Utilities|Casting|CastToBP_SGI (Game|GetGameInstance))
      (:then
        _)
      (:CastFailed
        _))
    (Variables|Default|SetSGI _asbp_sgi)
    (Utilities|IsOwner
      (:Server
        (Game|AssignOnDestroyed (delegate Custom|OnDestroyed_Event_0)))
      (:OwningClient
        (CallFunction|ClientSetRandomRotation)
        (EventDispatchers|AssignFormedChanged (Variables|/Game/Blueprints/BP_PAI.BP_PAI_C|GetIslandArchon (Variables|Default|GetBP_PAI)) (delegate Custom|Formed_Changed_Event_0))))))

(event Custom|Client_SetRandomRotation
  (bind _returnvalue (Math|Random|RandomFloatinRange 5.0 355.0))
  (Pawn|SetControlRotation (Variables|Default|GetBP_PCS) (Math|Rotator|MakeRotator 0.0 0.0 _returnvalue)) ; If rotation default = wind sound is freaking
  (Transformation|SetWorldRotation (Variables|Default|GetSkySpringArm1) (Math|Rotator|MakeRotator 0.0 -2e+01 _returnvalue) false false))

(event Custom|OpenCompleted)

(event Custom|Multicast_SpiritSpawnAnimation
  (params (Char_IslandRotation :type Rotator))
  (bind _spawntimeline (Variables|Default|GetSpawnTimeline))
  (Transformation|SetActorRotation Char_IslandRotation)
  (Rendering|SetVisibility (Variables|Default|GetSpiritBall) false false)
  (if (Class|LowEntryExtendedStandardLibrary|ShippingBuild)
    (Components|Timeline|SetPlayRate _spawntimeline 1.0)
    (bind _move (Timeline|SpawnTimeline PlayFromStart)
      (:Update
        (Transformation|SetRelativeLocation (Variables|Default|GetSpiritBall) (Spline|GetLocationatDistanceAlongSpline (Variables|Default|GetSpline) (Math|Float|Lerp 0.0 (Spline|GetSplineLength (Variables|Default|GetSpline)) _move) "Local") false false)
        (Class|CameraComponent|SetPostProcessBlendWeight (Variables|Default|GetCamera) (Math|Float|MapRangeClamped _move 0.0 1.0 1.0 0.0))
        (Rendering|Material|SetScalarParameterValue "/Game/GlobalMaterials/Col_Blur.Col_Blur" "BlurAmount" (Math|Float|MapRangeClamped _move 0.0 1.0 0.3 0.0) :!class /Script/Engine.KismetMaterialLibrary))
      (:Finished
        (Utilities|IsOwner
          (:OwningClient
            (CallFunction|ServerSwitch)))))
    (else
      (Components|Timeline|SetPlayRate _spawntimeline 1e+01)
      (Timeline|SpawnTimeline PlayFromStart))))

(event Custom|Server_Switch
  (bind _spawned_pf_normal (Variables|Default|GetSpawned_PF_Normal))
  (Rendering|SetActorHiddenInGame _spawned_pf_normal false)
  (Default|ServerAddIC _spawned_pf_normal)
  (CallFunction|MulticastDeactivate)
  (CallFunction|MulticastSNNormalEmerge _spawned_pf_normal)
  (Transformation|DetachFromActor (Variables|Default|GetSpawned_PF_Normal) "KeepWorld" "KeepWorld" "KeepWorld")
  (Default|PossessPawn (Variables|Default|GetBP_PCS) (Variables|Default|GetSpawned_PF_Normal) true)
  (Actor|DestroyActor))

(event Custom|Multicast_InitSetup
  (params (Essence :type Essence%20Structure) (Inventory :type Array%20of%20Inventory%20Slot%20Structures) (Equipment :type Array%20of%20Inventory%20Slot%20Structures))
  (Variables|Default|SetEssence Essence)
  (Variables|/Game/Blueprints/Inventory.Inventory_C|SetSlots (Variables|Default|GetInventory) Inventory)
  (Variables|/Game/Blueprints/Inventory.Inventory_C|SetSlots (Variables|Default|GetInventory_Equipment) Equipment))

(event Custom|Multicast_Deactivate
  (bind _sn_spiritspawn (Variables|Default|GetSN_SpiritSpawn))
  (if (not (Networking|IsDedicatedServer))
    (Utilities|IsValid _sn_spiritspawn
      (:Is%20Valid
        (Default|DeactivateAdianNiagara _sn_spiritspawn)))))

(event Custom|Multicast_SN_SpiritSpawn
  (if (not (Networking|IsDedicatedServer))
    (bind _returnvalue (Game|SpawnActorfromClass "/Game/Particles/AdianNiagara.AdianNiagara_C" (Math|Transform|MakeTransform "0, 0, 0" "0, 0, 0" "1.000000,1.000000,1.000000") "AlwaysSpawn" 0 "/Game/Particles/NS_Island_SpiritSpawn.NS_Island_SpiritSpawn" 0))
    (bind _output_get (Variables|Default|SetSN_SpiritSpawn _returnvalue))
    (Transformation|AttachComponentToComponent _output_get (Variables|Default|GetSpiritBall) "None" "KeepRelative" "KeepRelative" "KeepRelative" true)))

(event Custom|Multicast_SN_Normal_Emerge
  (params (PF_Normal :type PF%20Normal%20Object%20Reference))
  (Animation|Montage|PlayMontage (Variables|/Script/Engine.Character|GetMesh PF_Normal) "/Game/Characters/Animations/Male_Teleported_Montage.Male_Teleported_Montage"
    (:then
      (if (not (Networking|IsDedicatedServer))
        (bind _returnvalue (Game|SpawnActorfromClass "/Game/Particles/AdianNiagara.AdianNiagara_C" (Math|Transform|MakeTransform "0, 0, 0" "0, 0, 0" "1.000000,1.000000,1.000000") "AlwaysSpawn" 0 "/Game/Particles/NS_Normal_Emerge.NS_Normal_Emerge" 0))
        (Transformation|AttachActorToActor _returnvalue PF_Normal "None" "KeepRelative" "KeepRelative" "KeepRelative" true)))))

(event Custom|OnDestroyed_Event_0
  (params (DestroyedActor :type Actor%20Object%20Reference))
  (if (Variables|Default|GetEmerging)
    _))

(event EventClientUnpossess
  (Default|HideAnimation (Variables|Default|GetW_PF_Island) (delegate Custom|HideCompleted)))

(event EventBeginPlay
  (if (not (Variables|Default|GethadBeginPlay))
    (Variables|Default|SethadBeginPlay true)
    (bind _asbp_sgi (Utilities|Casting|CastToBP_SGI (Game|GetGameInstance))
      (:then
        _)
      (:CastFailed
        _))
    (Variables|Default|SetSGI _asbp_sgi)
    (Utilities|IsOwner
      (:Server
        (Game|AssignOnDestroyed (delegate Custom|OnDestroyed_Event_0)))
      (:OwningClient
        (CallFunction|ClientSetRandomRotation)
        (EventDispatchers|AssignFormedChanged (Variables|/Game/Blueprints/BP_PAI.BP_PAI_C|GetIslandArchon (Variables|Default|GetBP_PAI)) (delegate Custom|Formed_Changed_Event_0))))))

(event EventPossessed
  (params (NewController :type Controller%20Object%20Reference))
  (CallFunction|EnsureBeginPlay)
  (Default|MulticastPlayerFormPossessed (Variables|Default|GetBP_PAI) "Island" self)
  (CallFunction|ClientPossessed)
  (Game|Player|SetViewTargetwithBlend (Variables|Default|GetBP_PCS) self 0.0 "VTBlend_Linear" 0.0 false))

(event EventClientAfterPossess
  (bind _bp_pcs (Variables|Default|GetBP_PCS))
  (bind _w_eyestransition (Variables|/Game/Blueprints/BP_PCS.BP_PCS_C|GetW_EyesTransition _bp_pcs))
  (Default|CallAfterPFPossessed (Variables|Default|GetBP_PCS))
  (Rendering|Material|SetScalarParameterValue "/Game/GlobalMaterials/Col_Blur.Col_Blur" "BlurAmount" 0.3 :!class /Script/Engine.KismetMaterialLibrary)
  (bind _returnvalue (UserInterface|CreateWidget "/Game/Widgets/W_PF_Island.W_PF_Island_C" (Variables|Default|GetBP_PCS)))
  (bind _output_get (Variables|Default|SetW_PF_Island _returnvalue))
  (Default|ShowAnimation _output_get (delegate Custom|ShowCompleted))
  (UserInterface|Viewport|AddtoViewport _output_get 0)
  (Utilities|IsValid _w_eyestransition
    (:Is%20Valid
      (Default|OpenEyes _w_eyestransition (delegate Custom|OpenCompleted)))))

(event Input|ActionEvents|InputActionJump
  (params (Key :type Key%20Structure))
  (bind _returnvalue (Transformation|GetActorRotation))
  (bind _returnvalue_2 (Transformation|GetActorLocation))
  (bind _emergeprogress (Variables|Default|GetEmergeProgress))
  (bind _returnvalue_3 (Math|Vector|GetForwardVector (Math|Rotator|MakeRotator 0.0 0.0 (.yaw _returnvalue))))
  (bind _returnvalue_4 (+ _returnvalue_2 "0, 0,100.000000"))
  (bind _returnvalue_5 (* _returnvalue_3 2e+02))
  (bind _returnvalue_6 (+ _returnvalue_4 _returnvalue_5))
  (:Pressed
    (Utilities|Hold/Tap 0.15 :!label _label
      (:HoldStart
        (if (Class|LowEntryExtendedStandardLibrary|ShippingBuild)
          (Components|Timeline|SetPlayRate _emergeprogress 1.0)
          (bind _progressvalue (Timeline|EmergeProgress PlayFromStart)
            (:Update
              (Default|SetProgress (Variables|/Game/Widgets/W_PF_Island.W_PF_Island_C|GetReviveProgress (Variables|Default|GetW_PF_Island)) _progressvalue))
            (:Finished
              (bind (_outhit _returnvalue_7) (Collision|LineTraceByChannel _returnvalue_6 (+ _returnvalue_6 "0, 0,-400.000000") "TraceTypeQuery1" false 0 "None"))
              (if _returnvalue_7
                (CallFunction|ServerSpawnNormal (Math|Transform|MakeTransform (+ (.Location (Collision|BreakHitResult _outhit)) "0, 0,100.000000") (Transformation|GetActorRotation)))
                (Input|DisableInput self (Variables|Default|GetBP_PCS))
                (else
                  (Default|SetProgress (Variables|/Game/Widgets/W_PF_Island.W_PF_Island_C|GetReviveProgress (Variables|Default|GetW_PF_Island)) 0.0)))))
          (else
            (Components|Timeline|SetPlayRate _emergeprogress 1e+01)
            (Timeline|EmergeProgress PlayFromStart))))
      (:HoldStop
        (Default|SetProgress (Variables|/Game/Widgets/W_PF_Island.W_PF_Island_C|GetReviveProgress (Variables|Default|GetW_PF_Island)) 0.0)
        (Timeline|EmergeProgress Stop))))
  (:Released
    (goto _label Released)))

(event Input|ActionEvents|InputActionInventory
  (params (Key :type Key%20Structure))
  (:Pressed
    (bind _returnvalue (UserInterface|CreateWidget "/Game/Widgets/CWS/CWS_InventoryCharIsland.CWS_InventoryCharIsland_C" (Variables|Default|GetBP_PCS) self))
    (UserInterface|Viewport|AddtoViewport _returnvalue 0)
    (Default|AddCWS (Variables|Default|GetBP_PAI) _returnvalue true true "NewEnumerator2")))

(event Input|ActionEvents|InputActionInteract1
  (params (Key :type Key%20Structure))
  (bind _bp_pai (Variables|Default|GetBP_PAI))
  (:Pressed
    (Default|CreateMenu (Variables|/Game/Blueprints/BP_PAI.BP_PAI_C|GetIslandArchon _bp_pai) self _bp_pai)))

(event Input|AxisEvents|InputAxisLookUp
  (params (AxisValue :type Float%20%28single-precision%29))
  (bind _skyspringarm1 (Variables|Default|GetSkySpringArm1))
  (bind _returnvalue (Transformation|GetWorldRotation _skyspringarm1))
  (Transformation|SetWorldRotation (Variables|Default|GetSkySpringArm1) (Math|Rotator|MakeRotator (.roll _returnvalue) (Math|Float|ClampAngle (+ (* AxisValue -1.0) (.pitch _returnvalue)) -85.0 (Math|Float|SelectFloat 0.0 85.0 (Variables|/Game/Blueprints/IslandArchon.IslandArchon_C|GetCrystal (Variables|/Game/Blueprints/BP_PAI.BP_PAI_C|GetIslandArchon (Variables|Default|GetBP_PAI))))) (.yaw _returnvalue)) false false))

(event Input|AxisEvents|InputAxisTurn
  (params (AxisValue :type Float%20%28single-precision%29))
  (bind _returnvalue (Transformation|GetActorRotation))
  (Transformation|SetActorRotation (Math|Rotator|MakeRotator (.roll _returnvalue) (.pitch _returnvalue) (+ AxisValue (.yaw _returnvalue)))))

(fn ConstructionScript)

(fn SpawnPFNormal(Server)
  (params (SpawnTransform_Location :type Vector) (Char_IslandRotation :type Rotator))
  (bind _bp_pcs (Variables|Default|GetBP_PCS))
  (bind _returnvalue (Game|SpawnActorfromClass "/Game/Blueprints/PF_Normal.PF_Normal_C" (Math|Transform|MakeTransform SpawnTransform_Location (Math|Rotator|MakeRotator 0.0 0.0 (.Yaw (Math|Rotator|BreakRotator Char_IslandRotation))) "1.000000,1.000000,1.000000") "AdjustIfPossibleButAlwaysSpawn" _bp_pcs _bp_pcs (Variables|Default|GetBP_PAI) 0))
  (bind _output_get (Variables|Default|SetSpawned_PF_Normal _returnvalue))
  (Default|MulticastInitialization _output_get (Variables|/Game/Blueprints/BP_PCS.BP_PCS_C|GetS_CharacterBio (Variables|Default|GetBP_PCS)) (Variables|Default|GetEssence) (Variables|/Game/Blueprints/Inventory.Inventory_C|GetSlots (Variables|Default|GetInventory)) (Variables|/Game/Blueprints/Inventory.Inventory_C|GetSlots (Variables|Default|GetInventory_Equipment)))
  (Default|ClientSetLookRotation (Variables|Default|GetSpawned_PF_Normal) Char_IslandRotation)
  (Variables|Default|SetEmerging true)
  (Default|SpawnChunks (Variables|/Game/Blueprints/PF_Normal.PF_Normal_C|GetGenerator_Islands (Variables|Default|GetSpawned_PF_Normal)))
  (Default|MinusSpawnedChunks (Variables|Default|GetGenerator_Islands))
  (Default|SpawnChunks (Variables|/Game/Blueprints/PF_Normal.PF_Normal_C|GetGenerator_Essence (Variables|Default|GetSpawned_PF_Normal)))
  (Default|MinusSpawnedChunks (Variables|Default|GetGenerator_Essence))
  (Game|Player|SetViewTargetwithBlend (Variables|Default|GetBP_PCS) (Variables|Default|GetSpawned_PF_Normal) 1.0 "VTBlend_EaseInOut" 2.0 false)
  (CallFunction|MulticastSpiritSpawnAnimation Char_IslandRotation)
  (CallFunction|MulticastSNSpiritSpawn)
  (Default|MulticastSetAttachedtoIA (Variables|Default|GetSpawned_PF_Normal) (Variables|/Game/Blueprints/BP_PAI.BP_PAI_C|GetIslandArchon (Variables|Default|GetBP_PAI))))

(fn OnRepEssence
  (Default|CallEssenceChanged))

(fn RemoveWPFIsland
  (bind _w_pf_island (Variables|Default|GetW_PF_Island))
  (Utilities|IsValid _w_pf_island
    (:Is%20Valid
      (Widget|RemovefromParent _w_pf_island))))

(fn CameraComponents
  (return (Variables|Default|GetSkySpringArm) (Variables|Default|GetCamera)))

(fn GetBPPAI
  (return (Variables|Default|GetBP_PAI)))

(fn GetBPPCS
  (return (Variables|Default|GetBP_PCS)))

(fn GetInventory
  (return (Variables|Default|GetInventory)))

(fn GetPlayerForm
  (return self 0 0 0))

(fn GetLookRotation
  (return (Variables|Default|GetLookRotation)))

(fn SetLookRotation
  (params (LookRotation :type Rotator :default "0, 0, 0"))
  (bind _output_get (Variables|Default|SetLookRotation LookRotation))
  (return _output_get))