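; Physics-driven log that damages what it slams into and plays impact sound and camera shake.
; On the server, hard hits trigger an unreliable multicast for impulse-scaled FX.
; Damage also scales with impulse, requires the velocity cached on Tick to be fast and aimed into the surface, and has a per-actor cooldown.
; On spawn, Grimroot logs get a random horizontal push with matching spin to set them moving.
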(event Custom|Multicast_ImpactFX
  (params (WorldLocation :type Vector%20Net%20Quantize%20Structure) (NormalImpulseLength :type Float%20%28double-precision%29))
  (Audio|SpawnSoundAttached "/Game/Audio/SFX/LogImpact/Meta_PhysicsLog.Meta_PhysicsLog" (Variables|Default|GetStaticMeshComponent) "None" (Math|Transform|InverseTransformLocation (Transformation|GetWorldTransform (Variables|Default|GetStaticMeshComponent)) WorldLocation) "0, 0, 0" "KeepRelativeOffset" false (Math|Float|MapRangeClamped NormalImpulseLength 3e+05 6e+06 0.1 1.25) (Math|Float|MapRangeClamped NormalImpulseLength 3e+05 6e+06 0.75 1.25) 0.0 "/Game/Audio/BigAttenuation.BigAttenuation" 0)
  (Camera|PlayWorldCameraShake "/Game/Blueprints/CameraShake/CS_MediumImpact.CS_MediumImpact_C" WorldLocation 0.0 6e+03))

(event Collision|EventHit
  (params (MyComp :type Primitive%20Component%20Object%20Reference) (Other :type Actor%20Object%20Reference) (OtherComp :type Primitive%20Component%20Object%20Reference) (bSelfMoved :type Boolean) (HitLocation :type Vector :default "0, 0, 0") (HitNormal :type Vector :default "0, 0, 0") (NormalImpulse :type Vector :default "0, 0, 0") (Hit :type Hit%20Result%20Structure%20%28by%20ref%29))
  (bind (_bblockinghit _binitialoverlap _time _distance _location _impactpoint _normal _impactnormal) (Collision|BreakHitResult Hit))
  (bind _returnvalue (Math|Vector|VectorLength NormalImpulse))
  (bind _lasthittime (Variables|Default|GetLastHitTime))
  (bind (_value _returnvalue_2) (Utilities|Map|Find _lasthittime Other))
  (Networking|SwitchHasAuthority
    (:Authority
      (if (> _returnvalue 3e+05)
        (CallFunction|MulticastImpactFX (Class|AdianFL|ToQuantize(Vector) _impactpoint) _returnvalue)
        (if (> (Math|Vector|VectorLength (Variables|Default|GetTickVelocity)) 2e+02)
          (if (> (Math|Vector|DotProduct (* _impactnormal -1.0) (Math|Vector|Normalize (Variables|Default|GetTickVelocity))) 0.4)
            (if _returnvalue_2
              (if (> (- (Utilities|Time|GetTimeSeconds) _value) 1.0)
                (Class|AdianFL|DoDamage Other (Utilities|Struct|MakeDamageInfo "/Game/DataAssets/DamageAction/PhysicsLog.PhysicsLog" self _impactpoint (Class|AdianFL|NormalizetoRangeClamped _returnvalue 2e+05 8e+06)) :!label _label)
                (Utilities|Map|Add (Variables|Default|GetLastHitTime) Other (Utilities|Time|GetTimeSeconds)))
              (else
                (goto _label)))))))))

(event EventTick
  (params (DeltaSeconds :type Float%20%28single-precision%29))
  (Variables|Default|SetTickVelocity (Transformation|GetVelocity)))

(event EventBeginPlay)

(event EventOnSpawnLogic
  (bind _returnvalue (Math|Random|RandomUnitVector))
  (bind _staticmeshcomponent (Variables|Default|GetStaticMeshComponent))
  (if (== (Variables|Default|GetDA_Resource) "/Game/DataAssets/Resource/R_GrimrootLog.R_GrimrootLog")
    (bind _output_get (Variables|Default|SetSpawnImpulseDirection (* (Math|Vector|Normalize (Math|Vector|MakeVector (.x _returnvalue) (.y _returnvalue) 0.0)) 2e+02)))
    (Physics|AddImpulse _staticmeshcomponent (Math|Vector|MakeVector (.x _output_get) (.y _output_get) 0.0) "None" true)
    (Class|PrimitiveComponent|AddAngularImpulseinDegrees _staticmeshcomponent (Math|Vector|MakeVector (* (.y _output_get) -0.075) (* (.x _output_get) 0.075) 0.0) "None" true)))

(fn ConstructionScript)