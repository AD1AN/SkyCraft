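; AttackTracer is a component that detects hits during an attack by box tracing along its owner's forward vector.
; StartTracing stores the trace extents, binds the caller's event to the Attacked dispatcher and enables tick; StopTracing unbinds and disables it.
; Each tick runs a multi box trace aligned to owner yaw, firing Attacked once per newly hit actor via the HitActors list, with optional debug drawing.
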(event EventTick
  (params (DeltaSeconds :type Float%20%28single-precision%29))
  (bind _returnvalue (Components|GetOwner))
  (bind _returnvalue_2 (Transformation|GetActorForwardVector _returnvalue))
  (bind _returnvalue_3 (Transformation|GetActorLocation _returnvalue))
  (bind (_outhits _returnvalue_4) (Class|KismetSystemLibrary|BoxTraceMulti (+ _returnvalue_3 (* _returnvalue_2 (Variables|Default|GetStart))) (+ _returnvalue_3 (* _returnvalue_2 (Variables|Default|GetEnd))) (Variables|Default|GetHalfSize) (Math|Rotator|MakeRotator 0.0 0.0 (.yaw (Transformation|GetActorRotation (Components|GetOwner)))) "TraceTypeQuery5" false 0 (select (Variables|Default|GetDebug) "ForDuration" "None") true))
  (if _returnvalue_4
    (for _array_element _outhits
      (if (not (Utilities|Array|ContainsItem (Variables|Default|GetHitActors) (.HitActor (Collision|BreakHitResult _array_element))))
        (Utilities|Array|Add (Variables|Default|GetHitActors) (.HitActor (Collision|BreakHitResult _array_element)))
        (Default|CallAttacked (.HitActor (Collision|BreakHitResult _array_element)) (.Location (Collision|BreakHitResult _array_element)))))))

(fn StartTracing
  (params (Start :type Float%20%28double-precision%29) (End :type Float%20%28double-precision%29) (HalfSize :type Vector) (Event :type Delegate%20%28by%20ref%29))
  (Variables|Default|SetStart Start)
  (Variables|Default|SetEnd End)
  (Variables|Default|SetHalfSize HalfSize)
  (EventDispatchers|BindEventtoAttacked Event)
  (Utilities|Array|Clear (Variables|Default|GetHitActors))
  (Components|Tick|SetComponentTickEnabled true))

(fn StopTracing
  (EventDispatchers|UnbindallEventsfromAttacked)
  (Components|Tick|SetComponentTickEnabled false)
  (Utilities|Array|Clear (Variables|Default|GetHitActors)))