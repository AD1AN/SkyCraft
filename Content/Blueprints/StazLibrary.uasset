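; StazLibrary is a shared helper function library for the game's Essence, inventory, equipment and resource systems, plus general actor utilities.
; Essence helpers add, subtract, total and normalize red/green/blue values, while UniformMinusEssence spreads a deduction evenly across colors, dropping depleted ones.
; Other helpers find the root attach parent, measure distance in meters, break inventory slots, derive seeded random integers and map resource tags and equipment indices.
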(fn GetRootActor
  (params (StartActor :type Actor%20Object%20Reference))
  (bind _output_get (LocalVariables|SetCurrentParent StartActor))
  (LocalVariables|SetLastValidParent _output_get)
  (while (Utilities|IsValid (LocalVariables|GetCurrentParent))
    (bind _output_get_2 (LocalVariables|SetCurrentParent (Actor|GetAttachParentActor (LocalVariables|GetCurrentParent))))
    (Utilities|IsValid _output_get_2
      (:Is%20Valid
        (LocalVariables|SetLastValidParent (LocalVariables|GetCurrentParent)))))
  (return (LocalVariables|GetLastValidParent)))

(fn BreakSInventorySlot
  (params (S_InventorySlot :type S%20Inventory%20Slot%20Structure))
  (bind (_item _quantity _durability) (Utilities|Struct|BreakS_InventorySlot S_InventorySlot))
  (return (.datatable _item) (.rowname _item) _quantity _durability))

(fn AddEssence
  (params (1 :type S%20Essence%20Structure) (2 :type S%20Essence%20Structure))
  (bind (_red _green _blue) (Utilities|Struct|BreakS_Essence 1))
  (bind (_red_2 _green_2 _blue_2) (Utilities|Struct|BreakS_Essence 2))
  (return (Utilities|Struct|MakeS_Essence (+ _red _red_2) (+ _green _green_2) (+ _blue _blue_2))))

(fn SubtractEssence
  (params (1 :type S%20Essence%20Structure) (2 :type S%20Essence%20Structure))
  (bind (_red _green _blue) (Utilities|Struct|BreakS_Essence 1))
  (bind (_red_2 _green_2 _blue_2) (Utilities|Struct|BreakS_Essence 2))
  (return (Utilities|Struct|MakeS_Essence (- _red _red_2) (- _green _green_2) (- _blue _blue_2))))

(fn EssenceMax
  (params (Essence :type S%20Essence%20Structure))
  (return (Math|Conversions|ToFloat(Integer) (Math|Integer|Max(Integer) (.red Essence) (.green Essence) (.blue Essence)))))

(fn EssenceRGB
  (params (Essence :type S%20Essence%20Structure))
  (return (Math|Float|MapRangeClamped (Math|Conversions|ToFloat(Integer) (.red Essence)) 0.0 (CallFunction|EssenceMax Essence) 0.0 1.0) (Math|Float|MapRangeClamped (Math|Conversions|ToFloat(Integer) (.green Essence)) 0.0 (CallFunction|EssenceMax Essence) 0.0 1.0) (Math|Float|MapRangeClamped (Math|Conversions|ToFloat(Integer) (.blue Essence)) 0.0 (CallFunction|EssenceMax Essence) 0.0 1.0)))

(fn Int->Stream->Int
  (params (InitialSeed :type Integer))
  (return (Class|KismetMathLibrary|RandomIntegerfromStream 2147483647 (Math|Random|MakeRandomStream InitialSeed))))

(fn UniformMinusEssence
  (params (Essence :type S%20Essence%20Structure) (Minus :type Integer))
  (LocalVariables|SetTempEssence Essence)
  (LocalVariables|SetMinusLeft Minus)
  (while true
    (LocalVariables|SetUniformConsume (Math|Integer|SelectInt (/ (LocalVariables|GetMinusLeft) (Utilities|Array|Length (LocalVariables|GetEssenceColors))) 1 (> (/ (LocalVariables|GetMinusLeft) (Utilities|Array|Length (LocalVariables|GetEssenceColors))) 0)))
    (for _array_element (LocalVariables|GetEssenceColors)
      (bind _output_get (LocalVariables|SetElemColor _array_element))
      (LocalVariables|SetElemLeft (- (Utilities|Select :Index (- _output_get 1) :Option%200 (.red (LocalVariables|GetTempEssence)) :Option%201 (.green (LocalVariables|GetTempEssence)) :Option%202 (.blue (LocalVariables|GetTempEssence))) (LocalVariables|GetUniformConsume)))
      (if (>= (- (Utilities|Select :Index (- _output_get 1) :Option%200 (.red (LocalVariables|GetTempEssence)) :Option%201 (.green (LocalVariables|GetTempEssence)) :Option%202 (.blue (LocalVariables|GetTempEssence))) (LocalVariables|GetUniformConsume)) 0)
        (LocalVariables|SetMinusLeft (- (LocalVariables|GetMinusLeft) (LocalVariables|GetUniformConsume)))
        (if (== (LocalVariables|GetElemLeft) 0)
          (Utilities|Array|Add (LocalVariables|GetColorRemove) (LocalVariables|GetElemColor)))
        (else
          (LocalVariables|SetMinusLeft (- (LocalVariables|GetMinusLeft) (Utilities|Select :Index (- _output_get 1) :Option%200 (.red (LocalVariables|GetTempEssence)) :Option%201 (.green (LocalVariables|GetTempEssence)) :Option%202 (.blue (LocalVariables|GetTempEssence)))))
          (LocalVariables|SetElemLeft 0)
          (Utilities|Array|Add (LocalVariables|GetColorRemove) (LocalVariables|GetElemColor))))
      (switch int (- (LocalVariables|GetElemColor) 1)
        (:0
          (Utilities|Struct|SetmembersinS_Essence (LocalVariables|GetTempEssence) (LocalVariables|GetElemLeft)))
        (:1
          (Utilities|Struct|SetmembersinS_Essence (LocalVariables|GetTempEssence) (LocalVariables|GetElemLeft)))
        (:2
          (Utilities|Struct|SetmembersinS_Essence (LocalVariables|GetTempEssence) (LocalVariables|GetElemLeft))))
      (if (or (<= (LocalVariables|GetMinusLeft) 0) (== (Utilities|Array|Length (LocalVariables|GetEssenceColors)) 0))
        (return (LocalVariables|GetTempEssence))))
    (for _array_element_2 (LocalVariables|GetColorRemove)
      (Utilities|Array|RemoveItem (LocalVariables|GetEssenceColors) _array_element_2))
    (if (or (<= (LocalVariables|GetMinusLeft) 0) (== (Utilities|Array|Length (LocalVariables|GetEssenceColors)) 0))
      (return (LocalVariables|GetTempEssence)))))

(fn EssenceTotal
  (params (Essence :type S%20Essence%20Structure))
  (return (+ (.red Essence) (.green Essence) (.blue Essence))))

(fn DistanceMeters
  (params (A :type Actor%20Object%20Reference) (B :type Actor%20Object%20Reference))
  (return (Math|Float|Truncate (/ (Math|Vector|Distance(Vector) (Transformation|GetActorLocation A) (Transformation|GetActorLocation B)) 1e+02))))

(fn ResourceSTag->ResourceID
  (params (ResourceSTag :type Name))
  (switch name ResourceSTag
    (:Default
      _)
    (:Tree
      _)
    (:Stone
      (return 1))
    (:IronOre
      (return 1)))
  (return 0))

(fn EquipmentType
  (params (EQIndex :type Integer))
  (return (Utilities|Select :Index EQIndex :Option%200 "NewEnumerator4" :Option%201 "NewEnumerator5" :Option%202 "NewEnumerator10" :Option%203 "NewEnumerator7" :Option%204 "NewEnumerator8")))