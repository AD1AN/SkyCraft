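; Test actor that spawns a TEST_DeathEssence on its Island and hands that essence a new consume target when touched.
; On BeginPlay it spawns the essence with itself as ConsumeActor, passing along Character.
; The spawn location is pre-converted into Island local space so the keep-relative attachment to Island places it correctly.
; A mesh overlap sets ConsumeActor to the overlapping actor, then destroys this actor.
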(event OnComponentBeginOverlap(StaticMesh)
  (params (OverlappedComponent :type Primitive%20Component%20Object%20Reference) (OtherActor :type Actor%20Object%20Reference) (OtherComp :type Primitive%20Component%20Object%20Reference) (OtherBodyIndex :type Integer) (bFromSweep :type Boolean) (SweepResult :type Hit%20Result%20Structure%20%28by%20ref%29))
  (Variables|/Game/Blueprints/TEST_DeathEssence.TEST_DeathEssence_C|SetConsumeActor (Variables|Default|GetTestDeathEssence) OtherActor)
  (Actor|DestroyActor))

(event EventBeginPlay
  (bind _returnvalue (Game|SpawnActorfromClass "/Game/Blueprints/TEST_DeathEssence.TEST_DeathEssence_C" (Math|Transform|MakeTransform (Math|Transform|InverseTransformLocation (Transformation|GetActorTransform (Variables|Default|GetIsland)) (Transformation|GetActorLocation)) "0, 0, 0" "1.000000,1.000000,1.000000") "Undefined" "MultiplyWithRoot" 0 self (Variables|Default|GetCharacter) 0))
  (bind _output_get (Variables|Default|SetTestDeathEssence _returnvalue))
  (Transformation|AttachActorToActor _output_get (Variables|Default|GetIsland) "None" "KeepRelative" "KeepRelative" "KeepRelative" true))

(fn ConstructionScript)