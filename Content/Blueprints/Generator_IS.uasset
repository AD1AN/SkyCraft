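; Actor component that streams procedural sky-island chunks around its owner, running on the server in the Sky Main level.
; When the owner changes chunk coordinates, it releases chunks outside a circular radius and claims or spawns those inside, sharing them through GMSky with HMPR reference counts.
; Seeds from coordinates and WorldSeed decide which new chunks get islands and where, unless a saved location exists.
; Helpers report island counts to clients and transfer or release chunk claims.
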(event Custom|ForceBeginPlay
  (Variables|Default|SethadBeginPlay true)
  (Variables|Default|SetActor (Components|GetOwner))
  (bind _sgi (Class|BPISGI|GetSGI(Message) (Game|GetGameInstance)))
  (Variables|Default|SetSGI _sgi)
  (if (Networking|IsServer)
    (switch Utilities|FlowControl|Switch|SwitchonCurrentLevel (Variables|/Game/Blueprints/SGI.SGI_C|GetCurrentLevel (Variables|Default|GetSGI))
      (:NewEnumerator1
        (if (Class|LowEntryExtendedStandardLibrary|ShippingBuild)
          _
          (else
            (Variables|Default|SetShippingRenderRangeXY (Variables|Default|GetTestRenderRangeXY))))
        (bind _gm_sky (Class|BPIGameMS|GetGMSky(Message) (Game|GetGameMode)))
        (Variables|Default|SetGM_Sky _gm_sky)
        (Components|Tick|SetComponentTickEnabled true)))))

(event Custom|Server_ReturnIslands
  (bind _islands (CallFunction|ReturnIslands))
  (CallFunction|ClientReturnIslands _islands))

(event Custom|Client_ReturnIslands
  (params (Islands :type Integer))
  (Default|CallIslandsReturn (Variables|Default|GetSGI) Islands))

(event EventTick
  (params (DeltaSeconds :type Float%20%28single-precision%29))
  (bind (_x _y) (CallFunction|GetActorChunkCors))
  (bind (_x_2 _y_2) (CallFunction|GetActorChunkCors))
  (if (not (and (== _x_2 (.x (Variables|Default|GetLastActorChunkCors))) (== _y_2 (.y (Variables|Default|GetLastActorChunkCors))))) ; Player has changed Chunk Coordinates
    (Variables|Default|SetLastActorChunkCors (Utilities|Struct|MakeS_Int2Vector _x _y))
    (CallFunction|DestroyChunks)
    (CallFunction|SpawnChunks)))

(event EventBeginPlay
  (if (not (Variables|Default|GethadBeginPlay))
    (Variables|Default|SethadBeginPlay true)
    (Variables|Default|SetActor (Components|GetOwner))
    (bind _sgi (Class|BPISGI|GetSGI(Message) (Game|GetGameInstance)))
    (Variables|Default|SetSGI _sgi)
    (if (Networking|IsServer)
      (switch Utilities|FlowControl|Switch|SwitchonCurrentLevel (Variables|/Game/Blueprints/SGI.SGI_C|GetCurrentLevel (Variables|Default|GetSGI))
        (:NewEnumerator1
          (if (Class|LowEntryExtendedStandardLibrary|ShippingBuild)
            _
            (else
              (Variables|Default|SetShippingRenderRangeXY (Variables|Default|GetTestRenderRangeXY))))
          (bind _gm_sky (Class|BPIGameMS|GetGMSky(Message) (Game|GetGameMode)))
          (Variables|Default|SetGM_Sky _gm_sky)
          (Components|Tick|SetComponentTickEnabled true))))))

(fn GetActorChunkCors
  (bind _actor (Variables|Default|GetActor))
  (bind _chunksizexy (Variables|Default|GetChunkSizeXY))
  (bind _returnvalue (Transformation|GetActorLocation _actor))
  (bind _returnvalue_2 (/ _returnvalue _chunksizexy))
  (bind (_x _y) (Math|Vector|BreakVector _returnvalue_2))
  (return (Math|Float|Round _x) (Math|Float|Round _y)))

(fn DestroyChunks
  (bind (_x _y) (CallFunction|GetActorChunkCors))
  (bind _chunksizexy (Variables|Default|GetChunkSizeXY))
  (bind _chunksizexy_2 (Variables|Default|GetChunkSizeXY))
  (for (_array_element _array_index) (Variables|Default|GetHMPR_SpawnedChunksCors)
    (LocalVariables|SetTempIndex _array_index)
    (if (>= (Math|Vector|Distance(Vector) (Math|Vector|MakeVector (* (.X (Utilities|Struct|BreakS_Int2Vector _array_element)) _chunksizexy) (* (.Y (Utilities|Struct|BreakS_Int2Vector _array_element)) _chunksizexy) 0.0) (Math|Vector|MakeVector (* _x _chunksizexy_2) (* _y _chunksizexy_2) 0.0)) (* (Variables|Default|GetShippingRenderRangeXY) (Variables|Default|GetChunkSizeXY)))
      (Utilities|Array|Add (LocalVariables|GetIndexForRemoval) (LocalVariables|GetTempIndex))))
  (for (_array_element_2 _array_index_2) (LocalVariables|GetIndexForRemoval)
    (Variables|/Game/Blueprints/SA_Chunk_IS.SA_Chunk_IS_C|SetHMPR (Utilities|Array|Get(acopy) (Variables|Default|GetHMPR_SpawnedChunks) (- _array_element_2 _array_index_2)) (- (Variables|/Game/Blueprints/SA_Chunk_IS.SA_Chunk_IS_C|GetHMPR (Utilities|Array|Get(acopy) (Variables|Default|GetHMPR_SpawnedChunks) (- _array_element_2 _array_index_2))) 1))
    (Utilities|Array|RemoveIndex (Variables|Default|GetHMPR_SpawnedChunksCors) (- _array_element_2 _array_index_2))
    (Utilities|Array|RemoveIndex (Variables|Default|GetHMPR_SpawnedChunks) (- _array_element_2 _array_index_2))))

(fn SpawnChunks
  (bind (_x _y) (CallFunction|GetActorChunkCors))
  (bind _shippingrenderrangexy (Variables|Default|GetShippingRenderRangeXY))
  (bind _chunksizexy (Variables|Default|GetChunkSizeXY))
  (bind _chunksizexy_2 (Variables|Default|GetChunkSizeXY))
  (bind _gm_sky (Variables|Default|GetGM_Sky))
  (bind _shippingrenderrangexy_2 (Variables|Default|GetShippingRenderRangeXY))
  (bind _gm_sky_2 (Variables|Default|GetGM_Sky))
  (for _index (range (* _shippingrenderrangexy_2 -1) _shippingrenderrangexy_2)
    (LocalVariables|Set_TempX _index)
    (for _index_2 (range (* _shippingrenderrangexy -1) _shippingrenderrangexy)
      (LocalVariables|Set_TempY _index_2)
      (LocalVariables|Set_ChunkCors (Utilities|Struct|MakeS_Int2Vector (+ _x (LocalVariables|Get_TempX)) (+ _y (LocalVariables|Get_TempY))))
      (if (and (not (Utilities|Array|ContainsItem (Variables|Default|GetHMPR_SpawnedChunksCors) (LocalVariables|Get_ChunkCors))) (< (Math|Vector|VectorLength (Math|Vector|MakeVector (* (LocalVariables|Get_TempX) _chunksizexy) (* (LocalVariables|Get_TempY) _chunksizexy) 0.0)) (* (Variables|Default|GetShippingRenderRangeXY) (Variables|Default|GetChunkSizeXY))))
        (if (Utilities|Array|ContainsItem (Variables|/Game/Blueprints/GM_Sky.GM_Sky_C|GetSpawnedChunkIslandsCors (Variables|Default|GetGM_Sky)) (LocalVariables|Get_ChunkCors))
          (Utilities|Array|Add (Variables|Default|GetHMPR_SpawnedChunksCors) (LocalVariables|Get_ChunkCors))
          (Utilities|Array|Add (Variables|Default|GetHMPR_SpawnedChunks) (Utilities|Array|Get(acopy) (Variables|/Game/Blueprints/GM_Sky.GM_Sky_C|GetSpawnedChunkIslands _gm_sky_2) (Utilities|Array|FindItem (Variables|/Game/Blueprints/GM_Sky.GM_Sky_C|GetSpawnedChunkIslandsCors _gm_sky_2) (LocalVariables|Get_ChunkCors))))
          (Variables|/Game/Blueprints/SA_Chunk_IS.SA_Chunk_IS_C|SetHMPR (Utilities|Array|Get(acopy) (Variables|/Game/Blueprints/GM_Sky.GM_Sky_C|GetSpawnedChunkIslands _gm_sky_2) (Utilities|Array|FindItem (Variables|/Game/Blueprints/GM_Sky.GM_Sky_C|GetSpawnedChunkIslandsCors _gm_sky_2) (LocalVariables|Get_ChunkCors))) (+ (Variables|/Game/Blueprints/SA_Chunk_IS.SA_Chunk_IS_C|GetHMPR (Utilities|Array|Get(acopy) (Variables|/Game/Blueprints/GM_Sky.GM_Sky_C|GetSpawnedChunkIslands _gm_sky_2) (Utilities|Array|FindItem (Variables|/Game/Blueprints/GM_Sky.GM_Sky_C|GetSpawnedChunkIslandsCors _gm_sky_2) (LocalVariables|Get_ChunkCors)))) 1))
          (else
            (bind _returnvalue (Game|SpawnActorfromClass "/Game/Blueprints/SA_Chunk_IS.SA_Chunk_IS_C" (Math|Transform|MakeTransform (Math|Vector|MakeVector (* (.x (LocalVariables|Get_ChunkCors)) _chunksizexy_2) (* (.y (LocalVariables|Get_ChunkCors)) _chunksizexy_2) 5e+03) "0, 0, 0" "1.000000,1.000000,1.000000") "AlwaysSpawn" 0 (Variables|Default|GetGM_Sky) (CallFunction|Int->Stream->Int (+ (CallFunction|Int->Stream->Int (.x (LocalVariables|Get_ChunkCors))) (.y (LocalVariables|Get_ChunkCors)) (Variables|/Game/Blueprints/GM_Sky.GM_Sky_C|GetWorldSeed (Variables|Default|GetGM_Sky)))) 1 0))
            (LocalVariables|Set_SpawnedChunk _returnvalue)
            (Utilities|FlowControl|Sequence
              (:then_0
                (Utilities|Array|Add (Variables|/Game/Blueprints/GM_Sky.GM_Sky_C|GetSpawnedChunkIslands _gm_sky) (LocalVariables|Get_SpawnedChunk))
                (Utilities|Array|Add (Variables|/Game/Blueprints/GM_Sky.GM_Sky_C|GetSpawnedChunkIslandsCors _gm_sky) (LocalVariables|Get_ChunkCors))
                (Utilities|Array|Add (Variables|Default|GetHMPR_SpawnedChunks) (LocalVariables|Get_SpawnedChunk))
                (Utilities|Array|Add (Variables|Default|GetHMPR_SpawnedChunksCors) (LocalVariables|Get_ChunkCors)))
              (:then_1
                (if (Class|KismetMathLibrary|RandomBoolwithWeightfromStream 0.1 (Math|Random|MakeRandomStream (CallFunction|Int->Stream->Int (CallFunction|Int->Stream->Int (+ (CallFunction|Int->Stream->Int (.x (LocalVariables|Get_ChunkCors))) (.y (LocalVariables|Get_ChunkCors)) (Variables|/Game/Blueprints/GM_Sky.GM_Sky_C|GetWorldSeed (Variables|Default|GetGM_Sky)))))))
                  (if (.ReturnValue (Utilities|Map|Find (Variables|/Game/Blueprints/GM_Sky.GM_Sky_C|GetSavedIS (Variables|Default|GetGM_Sky)) (LocalVariables|Get_ChunkCors)))
                    (bind _returnvalue_2 (Game|SpawnActorfromClass "/Game/Blueprints/IslandStatic.IslandStatic_C" (Math|Transform|MakeTransform (.Location (Utilities|Struct|BreakSW_IslandStatic (.Value (Utilities|Map|Find (Variables|/Game/Blueprints/GM_Sky.GM_Sky_C|GetSavedIS (Variables|Default|GetGM_Sky)) (LocalVariables|Get_ChunkCors))))) "0, 0, 0" "1.000000,1.000000,1.000000") "AlwaysSpawn" 0 0))
                    (bind _output_get (Variables|/Game/Blueprints/SA_Chunk_IS.SA_Chunk_IS_C|SetIsland (LocalVariables|Get_SpawnedChunk) _returnvalue_2))
                    (Variables|/Game/Blueprints/IslandStatic.IslandStatic_C|SetChunk _output_get (LocalVariables|Get_SpawnedChunk))
                    (else
                      (Development|PrintString (Utilities|String|ToString(Float) (Math|Random|RandomFloatinRangefromStream (+ (* (.x (Components|Box|GetScaledBoxExtent (Variables|/Game/Blueprints/SA_Chunk_IS.SA_Chunk_IS_C|GetIslandBox (LocalVariables|Get_SpawnedChunk)))) -1.0) (.x (Transformation|GetWorldLocation (Variables|/Game/Blueprints/SA_Chunk_IS.SA_Chunk_IS_C|GetIslandBox (LocalVariables|Get_SpawnedChunk))))) (+ (.x (Components|Box|GetScaledBoxExtent (Variables|/Game/Blueprints/SA_Chunk_IS.SA_Chunk_IS_C|GetIslandBox (LocalVariables|Get_SpawnedChunk)))) (.x (Transformation|GetWorldLocation (Variables|/Game/Blueprints/SA_Chunk_IS.SA_Chunk_IS_C|GetIslandBox (LocalVariables|Get_SpawnedChunk))))) (Math|Random|MakeRandomStream (CallFunction|Int->Stream->Int (Variables|/Game/Blueprints/SA_Chunk_IS.SA_Chunk_IS_C|GetChunkSeed (LocalVariables|Get_SpawnedChunk)))))) true true "(R=0.000000,G=0.660000,B=1.000000,A=1.000000)" 555.0)
                      (bind _returnvalue_3 (Game|SpawnActorfromClass "/Game/Blueprints/IslandStatic.IslandStatic_C" (Math|Transform|MakeTransform (Math|Vector|MakeVector (Math|Random|RandomFloatinRangefromStream (+ (* (.x (Components|Box|GetScaledBoxExtent (Variables|/Game/Blueprints/SA_Chunk_IS.SA_Chunk_IS_C|GetIslandBox (LocalVariables|Get_SpawnedChunk)))) -1.0) (.x (Transformation|GetWorldLocation (Variables|/Game/Blueprints/SA_Chunk_IS.SA_Chunk_IS_C|GetIslandBox (LocalVariables|Get_SpawnedChunk))))) (+ (.x (Components|Box|GetScaledBoxExtent (Variables|/Game/Blueprints/SA_Chunk_IS.SA_Chunk_IS_C|GetIslandBox (LocalVariables|Get_SpawnedChunk)))) (.x (Transformation|GetWorldLocation (Variables|/Game/Blueprints/SA_Chunk_IS.SA_Chunk_IS_C|GetIslandBox (LocalVariables|Get_SpawnedChunk))))) (Math|Random|MakeRandomStream (CallFunction|Int->Stream->Int (Variables|/Game/Blueprints/SA_Chunk_IS.SA_Chunk_IS_C|GetChunkSeed (LocalVariables|Get_SpawnedChunk))))) (Math|Random|RandomFloatinRangefromStream (+ (* (.y (Components|Box|GetScaledBoxExtent (Variables|/Game/Blueprints/SA_Chunk_IS.SA_Chunk_IS_C|GetIslandBox (LocalVariables|Get_SpawnedChunk)))) -1.0) (.y (Transformation|GetWorldLocation (Variables|/Game/Blueprints/SA_Chunk_IS.SA_Chunk_IS_C|GetIslandBox (LocalVariables|Get_SpawnedChunk))))) (+ (.y (Components|Box|GetScaledBoxExtent (Variables|/Game/Blueprints/SA_Chunk_IS.SA_Chunk_IS_C|GetIslandBox (LocalVariables|Get_SpawnedChunk)))) (.y (Transformation|GetWorldLocation (Variables|/Game/Blueprints/SA_Chunk_IS.SA_Chunk_IS_C|GetIslandBox (LocalVariables|Get_SpawnedChunk))))) (Math|Random|MakeRandomStream (Variables|/Game/Blueprints/SA_Chunk_IS.SA_Chunk_IS_C|GetChunkSeed (LocalVariables|Get_SpawnedChunk)))) (Math|Random|RandomFloatinRangefromStream 7e+03 1.5e+04 (Math|Random|MakeRandomStream (Variables|/Game/Blueprints/SA_Chunk_IS.SA_Chunk_IS_C|GetChunkSeed (LocalVariables|Get_SpawnedChunk))))) "0, 0, 0" "1.000000,1.000000,1.000000") "AlwaysSpawn" 0 0))
                      (bind _output_get_2 (Variables|/Game/Blueprints/SA_Chunk_IS.SA_Chunk_IS_C|SetIsland (LocalVariables|Get_SpawnedChunk) _returnvalue_3))
                      (Variables|/Game/Blueprints/IslandStatic.IslandStatic_C|SetChunk _output_get_2 (LocalVariables|Get_SpawnedChunk)))))))))))))

(fn ReturnIslands
  (for _array_element (Variables|Default|GetHMPR_SpawnedChunks)
    (Utilities|IsValid (Variables|/Game/Blueprints/SA_Chunk_IS.SA_Chunk_IS_C|GetIsland _array_element)
      (:Is%20Valid
        (LocalVariables|Set_Islands (+ 1 (LocalVariables|Get_Islands))))))
  (return (LocalVariables|Get_Islands)))

(fn MinusSpawnedChunks
  (for _array_element (Variables|Default|GetHMPR_SpawnedChunks)
    (Variables|/Game/Blueprints/SA_Chunk_IS.SA_Chunk_IS_C|SetHMPR _array_element (- (Variables|/Game/Blueprints/SA_Chunk_IS.SA_Chunk_IS_C|GetHMPR _array_element) 1)))
  (Utilities|Array|Clear (Variables|Default|GetHMPR_SpawnedChunks))
  (Utilities|Array|Clear (Variables|Default|GetHMPR_SpawnedChunksCors)))

(fn TransferChunks
  (params (FromGenerator :type Generator%20IS%20Object%20Reference))
  (Variables|Default|SetHMPR_SpawnedChunks (Variables|Generator_IS_C|GetHMPR_SpawnedChunks FromGenerator))
  (Variables|Default|SetHMPR_SpawnedChunksCors (Variables|Generator_IS_C|GetHMPR_SpawnedChunksCors FromGenerator))
  (Variables|Default|SetLastActorChunkCors (Variables|Generator_IS_C|GetLastActorChunkCors FromGenerator))
  (return))