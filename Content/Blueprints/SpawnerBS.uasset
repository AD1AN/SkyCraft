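; SpawnerBS spawns snapping helper actors for nearby BP_BM buildings and can display their snap points.
; Sphere overlap spawns the BS class from the building's data asset, attaches it and links both ways; leaving the sphere destroys it.
; While snap display is on, VisualSnapBox actors attach to BS SnapBox components of the selected SnapType.
; Edit mode hides these visuals, changing display rebuilds them, and destroying the spawner removes them.
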(event OnComponentBeginOverlap(Sphere)
  (params (OverlappedComponent :type Primitive%20Component%20Object%20Reference) (OtherActor :type Actor%20Object%20Reference) (OtherComp :type Primitive%20Component%20Object%20Reference) (OtherBodyIndex :type Integer) (bFromSweep :type Boolean) (SweepResult :type Hit%20Result%20Structure%20%28by%20ref%29))
  (bind _asbp_bm (Utilities|Casting|CastToBP_BM OtherActor))
  (if (Utilities|IsValidClass (Variables|/Script/SkyCraft.DA_Building|GetBS_Class (Variables|/Script/SkyCraft.BM|GetDA_Building _asbp_bm)))
    (bind _returnvalue (Game|SpawnActorfromClass (Variables|/Script/SkyCraft.DA_Building|GetBS_Class (Variables|/Script/SkyCraft.BM|GetDA_Building _asbp_bm)) (Math|Transform|MakeTransform "0, 0, 0" "0, 0, 0" "1.000000,1.000000,1.000000") "AlwaysSpawn" "MultiplyWithRoot" 0 0))
    (Transformation|AttachActorToActor _returnvalue _asbp_bm "None" "KeepRelative" "KeepRelative" "KeepRelative" false)
    (bind _output_get (Variables|/Script/SkyCraft.BS|SetCurrentBM _returnvalue _asbp_bm))
    (bind _output_get_2 (Variables|/Script/SkyCraft.BM|SetCurrentBS _output_get _returnvalue))
    (Utilities|Array|Add (Variables|Default|GetSpawnedBS) _output_get_2)
    (CallFunction|SpawnVisualSnapBox _returnvalue)))

(event OnComponentEndOverlap(Sphere)
  (params (OverlappedComponent :type Primitive%20Component%20Object%20Reference) (OtherActor :type Actor%20Object%20Reference) (OtherComp :type Primitive%20Component%20Object%20Reference) (OtherBodyIndex :type Integer))
  (bind _asbp_bm (Utilities|Casting|CastToBP_BM OtherActor))
  (Utilities|IsValid (Variables|/Script/SkyCraft.BM|GetCurrentBS _asbp_bm)
    (:Is%20Valid
      (Utilities|Array|RemoveItem (Variables|Default|GetSpawnedBS) (Variables|/Script/SkyCraft.BM|GetCurrentBS _asbp_bm))
      (Actor|DestroyActor (Variables|/Script/SkyCraft.BM|GetCurrentBS _asbp_bm)))))

(event EventEndPlay
  (params (EndPlayReason :type EEndPlayReason%20Enum :default "Destroyed"))
  (switch Utilities|FlowControl|Switch|SwitchonEEndPlayReason EndPlayReason
    (:Destroyed
      (for _array_element (Variables|Default|GetSpawnedVisualSnapBoxes)
        (Utilities|IsValid _array_element
          (:Is%20Valid
            (Actor|DestroyActor _array_element))))
      (Utilities|Array|Clear (Variables|Default|GetSpawnedVisualSnapBoxes)))))

(fn ConstructionScript)

(fn ShowSnapBoxes
  (params (ShowSnapBoxes :type Boolean) (SnapType :type ESnapType%20Enum :default "Foundation"))
  (Variables|Default|SetShowingSnapBoxes ShowSnapBoxes)
  (Utilities|FlowControl|Sequence
    (:then_0
      (if (not (Utilities|Array|IsEmpty (Variables|Default|GetSpawnedVisualSnapBoxes)))
        (for _array_element (Variables|Default|GetSpawnedVisualSnapBoxes)
          (Utilities|IsValid _array_element
            (:Is%20Valid
              (Actor|DestroyActor _array_element))))
        (Utilities|Array|Clear (Variables|Default|GetSpawnedVisualSnapBoxes))))
    (:then_1
      (Variables|Default|SetSpawnedVisualSnapType SnapType)
      (if (Variables|Default|GetShowingSnapBoxes)
        (for _array_element_2 (Variables|Default|GetSpawnedBS)
          (CallFunction|SpawnVisualSnapBox _array_element_2))))))

(fn EditMode
  (params (EditMode :type Boolean))
  (Variables|Default|SetisEditMode EditMode)
  (for _array_element (Variables|Default|GetSpawnedVisualSnapBoxes)
    (Utilities|IsValid _array_element
      (:Is%20Valid
        (Rendering|SetActorHiddenInGame _array_element (Variables|Default|GetisEditMode))))))

(fn SpawnVisualSnapBox
  (params (BS :type Actor%20Object%20Reference))
  (Utilities|IsValid BS
    (:Is%20Valid
      (if (Variables|Default|GetShowingSnapBoxes)
        (bind _output_get (LocalVariables|Set_SnapBoxes (Actor|GetComponentsByClass BS "/Script/SkyCraft.SnapBox")))
        (for _array_element _output_get
          (if (Utilities|Enum|Equal(Enum) (Variables|/Script/SkyCraft.SnapBox|GetSnapType _array_element) (Variables|Default|GetSpawnedVisualSnapType))
            (bind _returnvalue (Game|SpawnActorfromClass "/Game/Blueprints/VisualSnapBox.VisualSnapBox_C" (Math|Transform|MakeTransform "0, 0, 0" "0, 0, 0" "1.000000,1.000000,1.000000") "AlwaysSpawn" "MultiplyWithRoot" 0 _array_element 0))
            (Utilities|Array|Add (Variables|Default|GetSpawnedVisualSnapBoxes) _returnvalue)
            (Transformation|AttachComponentToComponent _returnvalue _array_element "None" "KeepRelative" "KeepRelative" "KeepRelative" false)
            (Rendering|SetActorHiddenInGame _returnvalue (Variables|Default|GetisEditMode))))))))