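; Chunk island actor that sets its level of detail by grid distance to the nearest registered generator.
; UpdateLOD runs on BeginPlay and generator changes, taking the smallest Chebyshev distance, firing OnChangeLOD and forwarding it to IslandStatic.
; When its last generator leaves, it removes itself from BPGMS's spawned-island lists and destroys IslandStatic and itself.
; A LOD text handler exists, but its binding is disconnected.
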(event Custom|OnChangeLOD_Event
  (Rendering|Components|TextRender|SetText (Variables|Default|GettextLOD) (Utilities|Text|ToText(Integer) (Variables|Default|GetCurrentLOD))))

(event EventBeginPlay
  (CallFunction|UpdateLOD))

(fn ConstructionScript)

(fn DestroyChunk
  (bind _self self)
  (bind _islandstatic (Variables|Default|GetIslandStatic))
  (bind _bp_gms (Variables|Default|GetBP_GMS))
  (bind _bp_gms_2 (Variables|Default|GetBP_GMS))
  (bind _spawnedchunkislands (Variables|/Game/Blueprints/BP_GMS.BP_GMS_C|GetSpawnedChunkIslands _bp_gms_2))
  (bind _returnvalue (Utilities|Array|FindItem _spawnedchunkislands _self))
  (Utilities|Array|RemoveIndex (Variables|/Game/Blueprints/BP_GMS.BP_GMS_C|GetSpawnedChunkIslandsCors _bp_gms) _returnvalue)
  (Utilities|Array|RemoveIndex (Variables|/Game/Blueprints/BP_GMS.BP_GMS_C|GetSpawnedChunkIslands _bp_gms) _returnvalue)
  (Utilities|IsValid _islandstatic
    (:Is%20Valid
      (if (Class|VoxelWorld|IsCreated _islandstatic)
        (Class|VoxelWorld|DestroyWorld _islandstatic))
      (Actor|DestroyActor _islandstatic))
    (:Is%20Not%20Valid
      _))
  (Actor|DestroyActor))

(fn RemoveGenerator
  (params (Generator :type Chunker%20Islands%20Object%20Reference))
  (Utilities|Array|RemoveItem (Variables|Default|GetChunkers) Generator)
  (bind (_arrayindex _arrayelement) (Utilities|Array|ReverseforEachLoop (Variables|Default|GetChunkers))
    (:LoopBody
      (Utilities|IsValid _arrayelement
        (:Is%20Not%20Valid
          (Utilities|Array|RemoveIndex (Variables|Default|GetChunkers) _arrayindex))))
    (:Completed
      (if (Utilities|Array|IsEmpty (Variables|Default|GetChunkers))
        (CallFunction|DestroyChunk)
        (else
          (CallFunction|UpdateLOD))))))

(fn AddGenerator
  (params (Generator :type Chunker%20Islands%20Object%20Reference))
  (Utilities|Array|Add (Variables|Default|GetChunkers) Generator)
  (CallFunction|UpdateLOD))

(fn UpdateLOD
  (bind _islandstatic (Variables|Default|GetIslandStatic))
  (bind _coords (Variables|Default|GetCoords))
  (for _array_element (Variables|Default|GetChunkers)
    (bind _output_get (LocalVariables|Set_GenCoords (Default|GetCoords _array_element)))
    (if (or (< (Math|Integer|Max(Integer) (Math|Integer|Absolute(Integer) (- (.x _output_get) (.x _coords))) (Math|Integer|Absolute(Integer) (- (.y _output_get) (.y _coords)))) (LocalVariables|Get_LowestLOD)) (== (LocalVariables|Get_LowestLOD) -1))
      (LocalVariables|Set_LowestLOD (Math|Integer|Max(Integer) (Math|Integer|Absolute(Integer) (- (.x _output_get) (.x _coords))) (Math|Integer|Absolute(Integer) (- (.y _output_get) (.y _coords)))))))
  (if (> (LocalVariables|Get_LowestLOD) -1)
    (Variables|Default|SetCurrentLOD (LocalVariables|Get_LowestLOD))
    (Default|CallOnChangeLOD)
    (Utilities|IsValid _islandstatic
      (:Is%20Valid
        (Variables|/Script/SkyCraft.Island|SetCurrentLOD _islandstatic (LocalVariables|Get_LowestLOD))
        (Default|CallOnChangeLOD _islandstatic)))
    (else
      (Development|PrintString "ERROR: LowestLOD is -1. Something went wrong in UpdateLOD." true true "(R=1.000000,G=0.000000,B=0.028497,A=1.000000)" 15.0))))