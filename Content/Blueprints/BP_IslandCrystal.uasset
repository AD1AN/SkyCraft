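; Interactable crystal on a player island that opens the island's menu for the owning player.
; It caches the island as BP_PlayerIsland on the authority at begin and on clients through the PlayerIsland RepNotify.
; Client interaction creates the menu only if the interacting player's island matches this one.
; Server interaction attaches a Phantom-form pawn to the island, keeping world transform, and interruption detaches it.
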(event EventOnRepPlayerIsland
  (|CallParentFunction)
  (bind _asbp_player_island (Utilities|Casting|CastToBP_PlayerIsland (Variables|Default|GetPlayerIsland)))
  (Variables|Default|SetBP_IslandPlayer _asbp_player_island))

(event EventPostBeginActor
  (Networking|SwitchHasAuthority
    (:Authority
      (bind _asbp_player_island (Utilities|Casting|CastToBP_PlayerIsland (Variables|Default|GetPlayerIsland)))
      (Variables|Default|SetBP_IslandPlayer _asbp_player_island))))

(fn ConstructionScript)

(fn ClientInteractBP
  (params (InteractKey :type EInteractKey%20Enum :default "Interact1") (Pawn :type Pawn%20Object%20Reference) (BP_PSS :type BP%20PSS%20Object%20Reference))
  (if (== (Variables|/Game/Blueprints/BP_PSS.BP_PSS_C|GetBP_PlayerIsland BP_PSS) (Variables|Default|GetBP_IslandPlayer))
    (Default|CreateMenu (Variables|Default|GetBP_IslandPlayer) Pawn BP_PSS)))

(fn ClientInterruptBP
  (params (InterruptedBy :type EInterruptedBy%20Enum :default "Player") (InteractKey :type EInteractKey%20Enum :default "Interact1") (Pawn :type Pawn%20Object%20Reference) (BP_PSS :type BP%20PSS%20Object%20Reference))
  (return false))

(fn ServerInteractBP
  (params (InteractKey :type EInteractKey%20Enum :default "Interact1") (Pawn :type Pawn%20Object%20Reference) (BP_PSS :type BP%20PSS%20Object%20Reference))
  (switch Utilities|FlowControl|Switch|SwitchonEPlayerForm (Variables|/Script/SkyCraft.PSS|GetPlayerForm BP_PSS)
    (:Normal
      (return true))
    (:Phantom
      (Transformation|AttachActorToActor Pawn (Variables|Default|GetBP_IslandPlayer) "None" "KeepWorld" "KeepWorld" "KeepWorld" true)
      (return true))))

(fn ServerInterruptBP
  (params (InterruptedBy :type EInterruptedBy%20Enum :default "Player") (InteractKey :type EInteractKey%20Enum :default "Interact1") (Pawn :type Pawn%20Object%20Reference) (BP_PSS :type BP%20PSS%20Object%20Reference))
  (switch Utilities|FlowControl|Switch|SwitchonEPlayerForm (Variables|/Script/SkyCraft.PSS|GetPlayerForm BP_PSS)
    (:Normal
      (return true))
    (:Phantom
      (Transformation|DetachFromActor Pawn "KeepWorld" "KeepWorld" "KeepWorld")
      (return true))))