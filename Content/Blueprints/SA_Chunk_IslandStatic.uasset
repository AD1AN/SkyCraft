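; Island chunk actor that represents one grid cell, shows its LOD and coordinates as text, and manages the lifetime of its linked IslandStatic.
; It tracks the generators that reference it, pruning invalid ones on removal.
; An empty generator list or a non-positive Referenced RepNotify triggers DestroyChunk, which unregisters it from BPGMS and destroys the island and itself.
; LOD recalculation is stubbed: its generator loops do nothing.
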(event Custom|OnChangeLOD_Event
  (bind _coors (Variables|Default|Getcoors))
  (Rendering|Components|TextRender|SetText (Variables|Default|GettextLOD) (Utilities|Text|ToText(Integer) (Variables|Default|GetCurrentLOD)))
  (Rendering|Components|TextRender|SetText (Variables|Default|GettextCOORS) (Utilities|Text|ToText(String) (Utilities|String|Append "X:" (Utilities|String|ToString(Integer) (.x _coors)) " / " "Y:" (Utilities|String|ToString(Integer) (.y _coors))))))

(event EventBeginPlay
  (bind _coors (Variables|Default|Getcoors))
  (Rendering|Components|TextRender|SetText (Variables|Default|GettextLOD) (Utilities|Text|ToText(Integer) (Variables|Default|GetCurrentLOD)))
  (Rendering|Components|TextRender|SetText (Variables|Default|GettextCOORS) (Utilities|Text|ToText(String) (Utilities|String|Append "X:" (Utilities|String|ToString(Integer) (.x _coors)) " / " "Y:" (Utilities|String|ToString(Integer) (.y _coors))))))

(fn ConstructionScript)

(fn DestroyChunk
  (bind _self self)
  (bind _islandstatic (Variables|Default|GetIslandStatic))
  (bind _bp_gms (Variables|Default|GetBP_GMS))
  (bind _bp_gms_2 (Variables|Default|GetBP_GMS))
  (bind _spawnedchunkislands (Variables|/Game/Blueprints/BP_GMS.BP_GMS_C|GetSpawnedChunkIslands _bp_gms_2))
  (bind _returnvalue (Utilities|Array|FindItem _spawnedchunkislands _self))
  (Utilities|Array|RemoveIndex (Variables|/Game/Blueprints/BP_GMS.BP_GMS_C|GetSpawnedChunkIslandsCors _bp_gms) _returnvalue)
  (Utilities|Array|RemoveIndex (Variables|/Game/Blueprints/BP_GMS.BP_GMS_C|GetSpawnedChunkIslands _bp_gms) _returnvalue)
  (Utilities|IsValid _islandstatic
    (:Is%20Valid
      (Class|VoxelWorld|DestroyWorld _islandstatic)
      (Actor|DestroyActor _islandstatic))
    (:Is%20Not%20Valid
      _))
  (Actor|DestroyActor))

(fn OnRepReferenced
  (if (<= (Variables|Default|GetReferenced) 0)
    (CallFunction|DestroyChunk)))

(fn RemoveGenerator
  (params (Generator :type Generator%20Island%20Static%20Object%20Reference))
  (Utilities|Array|RemoveItem (Variables|Default|GetGenerators) Generator)
  (bind (_arrayindex _arrayelement) (Utilities|Array|ReverseforEachLoop (Variables|Default|GetGenerators))
    (:LoopBody
      (Utilities|IsValid _arrayelement
        (:Is%20Not%20Valid
          (Utilities|Array|RemoveIndex (Variables|Default|GetGenerators) _arrayindex))))
    (:Completed
      (if (Utilities|Array|IsEmpty (Variables|Default|GetGenerators))
        (CallFunction|DestroyChunk)))))

(fn AddGenerator
  (params (Generator :type Generator%20Island%20Static%20Object%20Reference) (LOD :type Integer))
  (Utilities|Array|Add (Variables|Default|GetGenerators) Generator)
  (for _array_element (Variables|Default|GetGenerators)
    _))

(fn UpdateLOD
  (for _array_element (Variables|Default|GetGenerators)
    _))