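; EditorSaving is an actor that provides an F4 hotkey to save the world and quit the game.
; On BeginPlay it caches the GMSky reference from the game mode through GetGMSkyMessage and enables input for player controller 0.
; F4 calls SaveWorld on that reference, then immediately quits; the IsServer check on BeginPlay leads to no logic.
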(event EventBeginPlay
  (bind _gm_sky (Class|BPIGameMS|GetGMSky(Message) (Game|GetGameMode)))
  (Variables|Default|SetGM%20Sky _gm_sky)
  (Input|EnableInput (Game|GetPlayerController 0))
  (if (Networking|IsServer)
    _))

(event Input|KeyboardEvents|F4
  (params (Key :type Key%20Structure :default "None"))
  (:Pressed
    (Default|SaveWorld (Variables|Default|GetGM%20Sky) true)
    (Game|QuitGame 0 "Quit" false)))

(fn ConstructionScript)