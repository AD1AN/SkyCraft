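; BP_Essence is an essence pickup actor that hands its Essence to the actor that overlaps it.
; On BeginPlay it tints a dynamic mesh material and its Niagara effect from the Essence value.
; Server-side overlap with an interact-proximity component or IslandArchon-tagged actor sends the consume message and destroys the pickup; only the former multicasts an attached, custom-depth consume effect.
; DestroyEssence removes it after a short random delay.
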(event OnComponentBeginOverlap(Mesh)
  (params (OverlappedComponent :type Primitive%20Component%20Object%20Reference) (OtherActor :type Actor%20Object%20Reference) (OtherComp :type Primitive%20Component%20Object%20Reference) (OtherBodyIndex :type Integer) (bFromSweep :type Boolean) (SweepResult :type Hit%20Result%20Structure%20%28by%20ref%29))
  (if (Networking|IsServer)
    (if (Components|ComponentHasTag OtherComp "InteractProximity_Collision")
      (Class|BPIEssence|ConsumeEssence(Message) OtherActor (Variables|Default|GetEssence))
      (CallFunction|MulticastNiagaraConsume OtherActor)
      (Actor|DestroyActor)
      (elif (Class|AdianFL|ActorHasSkyTag OtherActor "/Game/DataAssets/SkyTag/IslandArchon.IslandArchon")
        (Class|BPIEssence|ConsumeEssence(Message) OtherActor (Variables|Default|GetEssence))
        (Actor|DestroyActor)))))

(event Custom|Multicast_NiagaraConsume
  (params (ParentActor :type Actor%20Object%20Reference))
  (bind _returnvalue (Niagara|SpawnSystemAttached "/Game/Niagara/NS_Spirit_EssenceConsume.NS_Spirit_EssenceConsume" (Variables|/Script/Engine.Actor|GetRootComponent ParentActor) "None" "0, 0, 0" "0, 0, 0" "KeepRelativeOffset" true))
  (Niagara|SetNiagaraVariable(LinearColor) _returnvalue "EssenceColor" (Class|AdianFL|EssencetoRGB (Variables|Default|GetEssence)))
  (Rendering|SetRenderCustomDepth _returnvalue true)
  (Rendering|SetCustomDepthStencilValue _returnvalue 1))

(event Custom|DestroyEssence
  (Utilities|FlowControl|Delay (Math|Random|RandomFloatinRange 0.5 2.0))
  (Actor|DestroyActor))

(event EventBeginPlay
  (bind _returnvalue (Rendering|Material|CreateDynamicMaterialInstance (Variables|Default|GetMesh) 0 "/Game/MaterialsGlobal/M_Essence.M_Essence" "None" :!class /Script/Engine.PrimitiveComponent))
  (Rendering|Material|SetVectorParameterValue _returnvalue "EssenceColor" (Class|AdianFL|EssencetoRGB (Variables|Default|GetEssence)) :!class /Script/Engine.MaterialInstanceDynamic)
  (Niagara|SetNiagaraVariable(LinearColor) (Variables|Default|GetNiagara) "EssenceColor" (Class|AdianFL|EssencetoRGB (Variables|Default|GetEssence))))

(fn ConstructionScript)