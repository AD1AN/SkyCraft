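; Equipment inventory whose slots each accept only items of a matching equipment type.
; CanDropIn looks up the item's data table row and compares its Type with the target slot's EquipmentType, rejecting missing rows.
; Server_DropIn repeats that check, then swaps the whole slot contents between this inventory and the dragged one through ServerSAEInventory, ignoring the dragged quantity.
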(event EventBeginPlay)

(event EventTick
  (params (DeltaSeconds :type Float%20%28single-precision%29))
  (|CallParentFunction DeltaSeconds) ; This node is disabled and will not be called.\nDrag off pins to build functionality.
)

(fn CanDropin
  (params (S_InventorySlot :type S%20Inventory%20Slot%20Structure) (DropIn_SlotIndex :type Integer))
  (bind _item (Utilities|Struct|BreakS_InventorySlot S_InventorySlot))
  (bind _returnvalue (Utilities|GetDataTableRow (.datatable _item) (.rowname _item))
    (:then
      (return (Utilities|Enum|Equal(Enum) (.Type (Utilities|Struct|BreakS_Item _returnvalue)) (CallFunction|EquipmentType DropIn_SlotIndex))))
    (:RowNotFound
      (return false))))

(fn ServerDropin
  (params (SlotIndex :type Integer) (Dragged_Inventory :type Inventory%20Object%20Reference) (Dragged_SlotIndex :type Integer) (Dragged_Quantity :type Integer))
  (bind _inventoryslots (Variables|/Game/Blueprints/Inventory.Inventory_C|GetInventorySlots Dragged_Inventory))
  (bind _output (Utilities|Array|Get(acopy) _inventoryslots Dragged_SlotIndex))
  (bind (_datatable _rowname) (Utilities|Struct|BreakDataTableRowHandle (.item _output)))
  (bind _returnvalue (Utilities|GetDataTableRow _datatable _rowname)
    (:then
      (if (Utilities|Enum|Equal(Enum) (.Type (Utilities|Struct|BreakS_Item _returnvalue)) (CallFunction|EquipmentType SlotIndex))
        (LocalVariables|SetItem (Utilities|Array|Get(acopy) (Variables|Default|GetInventorySlots) SlotIndex))
        (CallFunction|ServerSAEInventory SlotIndex (Utilities|Array|Get(acopy) (Variables|/Game/Blueprints/Inventory.Inventory_C|GetInventorySlots Dragged_Inventory) Dragged_SlotIndex))
        (Default|ServerSAEInventory Dragged_Inventory Dragged_SlotIndex (LocalVariables|GetItem))))))