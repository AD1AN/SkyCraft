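; DamageSystem holds Health and applies typed damage to it, reporting whether damage landed and whether it was lethal.
; GetNegate selects a Negate multiplier for each global damage type, spanning physical, elemental, essence, velocity and pure.
; ApplyDamageBasic looks up the causer's indexed type, multiplies base damage by that factor and truncates it.
; Only positive results reduce Health, flagging destruction at zero or below.
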(fn GetNegate
  (params (DamageGlobalType :type EDamageGlobalType%20Enum :default "Slash"))
  (return (Utilities|Select :Index DamageGlobalType :Slash (Variables|DamageSystemNegations|GetNegate_Slash) :Thrust (Variables|DamageSystemNegations|GetNegate_Thrust) :Strike (Variables|DamageSystemNegations|GetNegate_Strike) :Fire (Variables|DamageSystemNegations|GetNegate_Fire) :Ice (Variables|DamageSystemNegations|GetNegate_Ice) :PositiveLightning (Variables|DamageSystemNegations|GetNegate_PositiveLightning) :NegativeLightning (Variables|DamageSystemNegations|GetNegate_NegativeLightning) :PositiveEssence (Variables|DamageSystemNegations|GetNegate_PositiveEssence) :NegativeEssence (Variables|DamageSystemNegations|GetNegate_NegativeEssence) :Velocity (Variables|DamageSystemNegations|GetNegate_Velocity) :Pure (Variables|DamageSystemNegations|GetNegate_Pure))))

(fn ApplyDamageBasic
  (params (In :type Apply%20Damage%20in%20Structure))
  (bind _negate (CallFunction|GetNegate (Utilities|Array|Get(acopy) (Variables|/Script/SkyCraft.DA_DamageCauserInfo|GetDamageGlobalTypes (.damagecauserinfo In)) (.indexdamageglobaltype In))))
  (bind _output_get (LocalVariables|Set_NegatedDamage (Math|Float|Truncate (* _negate (.BaseDamage (Utilities|Struct|BreakApplyDamageIn In))))))
  (if (> _output_get 0)
    (bind _output_get_2 (Variables|DamageSystemInfo|SetHealth (- (Variables|DamageSystemInfo|GetHealth) (LocalVariables|Get_NegatedDamage))))
    (if (<= _output_get_2 0)
      (return (Utilities|Struct|MakeApplyDamageOut true true))
      (else
        (return (Utilities|Struct|MakeApplyDamageOut true false))))
    (else
      (return ""))))