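; An actor component that makes an IslandArchon burn Essence to stay in existence, destructing it when none is left.
; On the server at BeginPlay it caches its owning Archon, binds to its formed-changed event, and sets component tick from the Archon's Crystal value, refreshing it on each change.
; Each tick either destructs the Archon if total Essence is depleted or applies a fixed uniform Essence deduction, without delta-time scaling.
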(event Custom|Formed_Changed_Event_0
  (Components|Tick|SetComponentTickEnabled (Variables|/Game/Blueprints/IslandArchon.IslandArchon_C|GetCrystal (Variables|Default|GetIslandArchon))))

(event EventBeginPlay
  (if (Networking|IsServer)
    (bind _asisland_archon (Utilities|Casting|CastToIslandArchon (Components|GetOwner))
      (:then
        _)
      (:CastFailed
        _))
    (bind _output_get (Variables|Default|SetIslandArchon _asisland_archon))
    (EventDispatchers|AssignFormedChanged _output_get (delegate Custom|Formed_Changed_Event_0))
    (Components|Tick|SetComponentTickEnabled (Variables|/Game/Blueprints/IslandArchon.IslandArchon_C|GetCrystal (Variables|Default|GetIslandArchon)))))

(event EventTick
  (params (DeltaSeconds :type Float%20%28single-precision%29))
  (bind _islandarchon (Variables|Default|GetIslandArchon))
  (if (<= (CallFunction|EssenceTotal (Variables|/Game/Blueprints/IslandArchon.IslandArchon_C|GetEssence (Variables|Default|GetIslandArchon))) 0)
    (Default|Destruct (Variables|Default|GetIslandArchon))
    (else
      (bind _finalessence (CallFunction|UniformMinusEssenceOLD (Variables|/Game/Blueprints/IslandArchon.IslandArchon_C|GetEssence _islandarchon) 3))
      (Variables|/Game/Blueprints/IslandArchon.IslandArchon_C|SetEssence _islandarchon _finalessence))))