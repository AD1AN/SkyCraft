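; Voxel world actor that generates a sky island for its replicated Chunk.
; When Chunk replicates, it feeds seed and scale to the generator, raises render octree depth for large islands, then creates the world.
; SpawnResources only debug-draws a grid of downward traces over the scaled chunk area, spawning nothing.
; Its world-loaded binding and the server/client spawner config selection are disconnected.
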(event Custom|OnWorldLoaded_Event_0
  (CallFunction|SpawnResources 100))

(event EventBeginPlay)

(fn ConstructionScript)

(fn OnRepChunk
  (bind _chunk (Variables|Default|GetChunk))
  (bind _chunkislandscale (Variables|/Game/Blueprints/SA_Chunk_IslandStatic.SA_Chunk_IslandStatic_C|GetChunkIslandScale _chunk))
  (Class|VoxelGeneratorTools|SetGeneratorParameter (Variables|Default|GetGenerator) "SeedName" (Variables|/Game/Blueprints/SA_Chunk_IslandStatic.SA_Chunk_IslandStatic_C|GetChunkSeed (Variables|Default|GetChunk)))
  (Class|VoxelGeneratorTools|SetGeneratorParameter (Variables|Default|GetGenerator) "Scale" _chunkislandscale)
  (if (> _chunkislandscale 170)
    (Class|VoxelWorld|SetRenderOctreeDepth 5))
  (Class|VoxelWorld|CreateWorld self))

(fn SpawnResources
  (params (SpawnPoints :type Integer))
  (bind _chunk (Variables|Default|GetChunk))
  (bind _chunk_2 (Variables|Default|GetChunk))
  (bind _chunk_3 (Variables|Default|GetChunk))
  (bind _gm_sky (Variables|/Game/Blueprints/SA_Chunk_IslandStatic.SA_Chunk_IslandStatic_C|GetGM_Sky _chunk))
  (bind _gm_sky_2 (Variables|/Game/Blueprints/SA_Chunk_IslandStatic.SA_Chunk_IslandStatic_C|GetGM_Sky _chunk_3))
  (bind _chunkislandscaleratio (Variables|/Game/Blueprints/SA_Chunk_IslandStatic.SA_Chunk_IslandStatic_C|GetChunkIslandScaleRatio _chunk_2))
  (bind _returnvalue (Math|Float|Clamp(Float) _chunkislandscaleratio 0.4 0.8))
  (bind _chunksizexy (Variables|/Game/Blueprints/GM_Sky.GM_Sky_C|GetChunkSizeXY _gm_sky))
  (bind _chunksizexy_2 (Variables|/Game/Blueprints/GM_Sky.GM_Sky_C|GetChunkSizeXY _gm_sky_2))
  (bind _returnvalue_2 (/ _chunksizexy 2.0))
  (bind _returnvalue_3 (* _returnvalue_2 _returnvalue))
  (LocalVariables|Set_GridSize (Math|Float|Sqrt (Math|Conversions|ToFloat(Integer) SpawnPoints)))
  (for _index (range 0 (- (Math|Float|Truncate (LocalVariables|Get_GridSize)) 1))
    (LocalVariables|Set_Row _index)
    (for _index_2 (range 0 (- (Math|Float|Truncate (LocalVariables|Get_GridSize)) 1))
      (LocalVariables|Set_Column _index_2)
      (Collision|LineTraceByChannel (- (+ (Math|Vector|MakeVector (* (+ (* (/ _chunksizexy_2 (LocalVariables|Get_GridSize)) (LocalVariables|Get_Column)) (* (/ _chunksizexy_2 (LocalVariables|Get_GridSize)) 0.5)) _returnvalue) (* (+ (* (/ _chunksizexy_2 (LocalVariables|Get_GridSize)) (LocalVariables|Get_Row)) (* (/ _chunksizexy_2 (LocalVariables|Get_GridSize)) 0.5)) _returnvalue) 2.5e+04) (Transformation|GetActorLocation (Variables|Default|GetChunk))) (Math|Vector|MakeVector _returnvalue_3 _returnvalue_3 0.0)) (+ (- (+ (Math|Vector|MakeVector (* (+ (* (/ _chunksizexy_2 (LocalVariables|Get_GridSize)) (LocalVariables|Get_Column)) (* (/ _chunksizexy_2 (LocalVariables|Get_GridSize)) 0.5)) _returnvalue) (* (+ (* (/ _chunksizexy_2 (LocalVariables|Get_GridSize)) (LocalVariables|Get_Row)) (* (/ _chunksizexy_2 (LocalVariables|Get_GridSize)) 0.5)) _returnvalue) 2.5e+04) (Transformation|GetActorLocation (Variables|Default|GetChunk))) (Math|Vector|MakeVector _returnvalue_3 _returnvalue_3 0.0)) "0,0,-25000.000000") "TraceTypeQuery1" false 0 "ForDuration" false "(R=1.000000,G=0.000000,B=0.000000,A=1.000000)" "(R=0.000000,G=1.000000,B=0.000000,A=1.000000)" 555.0))))