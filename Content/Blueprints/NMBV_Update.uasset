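; Actor component that keeps a pooled nav mesh bounds volume updated for its moving owner.
; On server BeginPlay it enables tick and borrows a scaled volume from the GMSky object obtained through the game mode, releasing it on EndPlay.
; Tick tracks the owner's XY movement and, beyond an update distance, notifies the navigation system that the volume's bounds changed, printing debug or error text.
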(event EventBeginPlay
  (if (Networking|IsServer)
    (Components|Tick|SetComponentTickEnabled true)
    (bind _gm_sky (Class|BPIGameMS|GetGMSky(Message) (Game|GetGameMode)))
    (bind _output_get (Variables|Default|SetGM_Sky _gm_sky))
    (bind _nmbv (Default|NMBVUse _output_get (Components|GetOwner) (Variables|Default|GetScaleNMBV)))
    (Variables|Default|SetNMBV _nmbv)))

(event EventTick
  (params (DeltaSeconds :type Float%20%28single-precision%29))
  (bind _returnvalue (Components|GetOwner))
  (bind _returnvalue_2 (Components|GetOwner))
  (bind _returnvalue_3 (Class|NavigationSystemV1|GetNavigationSystem))
  (bind _returnvalue_4 (Components|GetOwner))
  (bind _returnvalue_5 (Transformation|GetActorLocation _returnvalue_4))
  (bind _returnvalue_6 (Transformation|GetActorLocation _returnvalue_2))
  (if (> (Math|Vector|Distance(Vector) (Math|Vector|MakeVector (.x (Variables|Default|GetLastLocation)) (.y (Variables|Default|GetLastLocation)) 0.0) (Math|Vector|MakeVector (.x _returnvalue_5) (.y _returnvalue_5) 0.0)) (Variables|Default|GetUpdateDistance))
    (Variables|Default|SetLastLocation (Math|Vector|MakeVector (.x _returnvalue_6) (.y _returnvalue_6) 0.0))
    (Utilities|IsValid (Variables|Default|GetNMBV)
      (:Is%20Valid
        (Class|NavigationSystemV1|OnNavigationBoundsUpdated _returnvalue_3 (Variables|Default|GetNMBV))
        (Development|PrintString (Utilities|String|Append (Utilities|GetDisplayName _returnvalue) " : " (Utilities|GetDisplayName _returnvalue_3)) true true "(R=0.000000,G=1.000000,B=0.112817,A=1.000000)"))
      (:Is%20Not%20Valid
        (Development|PrintString (Utilities|String|Append "ERROR: NMBV not found in " (Utilities|GetDisplayName _returnvalue)) true true "(R=1.000000,G=0.000000,B=0.000000,A=1.000000)" 1e+01)))))

(event EventEndPlay
  (params (EndPlayReason :type EEndPlayReason%20Enum :default "Destroyed"))
  (if (Networking|IsServer)
    (Default|NMBVUnuse (Variables|Default|GetGM_Sky) (Variables|Default|GetNMBV))))