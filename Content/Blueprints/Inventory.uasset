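; Slot-based inventory that syncs items, quantities and per-slot properties across the network through server events and multicasts that fire change callbacks.
; Adding tops up matching stacks up to the item data asset's max before filling empty slots, while helpers remove, consume and count items.
; Drag and drop within or between inventories moves, merges or swaps slots, gated by CanDropIn, which always allows here.
; The slot UI functions are stubs.
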(event Custom|Multicast_Remove
  (params (RemoveIndex :type Byte))
  (Utilities|Array|RemoveIndex (Variables|Default|GetSlots) (Math|Conversions|ToInteger(Byte) RemoveIndex))
  (Default|CallOnRemove RemoveIndex))

(event Custom|Multicast_SAE
  (params (SlotIndex :type Byte) (InventorySlot :type Inventory%20Slot%20Structure))
  (Utilities|Array|SetArrayElem (Variables|Default|GetSlots) (Math|Conversions|ToInteger(Byte) SlotIndex) InventorySlot)
  (Default|CallOnSlotChanged SlotIndex))

(event Custom|Multicast_Append
  (params (Item :type Inventory%20Slot%20Structure%20%28by%20ref%29))
  (bind _returnvalue (Utilities|Array|Add (Variables|Default|GetSlots) Item))
  (Default|CallOnAppend (Math|Conversions|ToByte(Integer) _returnvalue)))

(event Custom|Server_SAE
  (params (SlotIndex :type Byte) (InventorySlot :type Inventory%20Slot%20Structure))
  (CallFunction|MulticastSAE SlotIndex InventorySlot))

(event Custom|Server_Add
  (params (InventorySlot :type Inventory%20Slot%20Structure))
  (CallFunction|Add InventorySlot))

(event Custom|Server_SAE_Property
  (params (SlotIndex :type Byte) (PropertyIndex :type Byte) (Property :type Item%20Property%20Structure))
  (CallFunction|MulticastSAEProperty SlotIndex PropertyIndex Property))

(event Custom|Multicast_SAE_Property
  (params (SlotIndex :type Byte) (PropertyIndex :type Byte) (Property :type Item%20Property%20Structure))
  (Utilities|Array|SetArrayElem (.Properties (Utilities|Struct|BreakInventorySlot (Utilities|Array|Get(acopy) (Variables|Default|GetSlots) (Math|Conversions|ToInteger(Byte) SlotIndex)))) (Math|Conversions|ToInteger(Byte) PropertyIndex) Property)
  (Default|CallOnSlotChanged SlotIndex))

(event Custom|Server_ADD_Property
  (params (Property :type Item%20Property%20Structure) (SlotIndex :type Byte))
  (CallFunction|MulticastADDProperty Property SlotIndex))

(event Custom|Multicast_ADD_Property
  (params (Property :type Item%20Property%20Structure) (SlotIndex :type Byte))
  (Utilities|Array|Add (.properties (Utilities|Array|Get(acopy) (Variables|Default|GetSlots) (Math|Conversions|ToInteger(Byte) SlotIndex))) Property))

(event Custom|Multicast_Add
  (params (InventorySlot :type Inventory%20Slot%20Structure))
  (Default|CallOnAdd InventorySlot))

(event EventTick
  (params (DeltaSeconds :type Float%20%28single-precision%29)))

(fn Add
  (params (InventorySlot :type Inventory%20Slot%20Structure))
  (bind (_da_item _quantity _properties) (Utilities|Struct|BreakInventorySlot InventorySlot))
  (bind (_success _quantity_2) (CallFunction|Add(Internal) InventorySlot))
  (Utilities|FlowControl|Sequence
    (:then_0
      (if _success
        (CallFunction|MulticastAdd (Utilities|Struct|MakeInventorySlot _da_item _quantity_2 _properties))))
    (:then_1
      (return _success _quantity_2))))

(fn Add(Internal)
  (params (InventorySlot :type Inventory%20Slot%20Structure))
  (bind (_da_item _quantity) (Utilities|Struct|BreakInventorySlot InventorySlot))
  (LocalVariables|Set_DA_Item _da_item)
  (LocalVariables|Set_LeftQuantity _quantity)
  (if (Variables|/Script/SkyCraft.DA_Item|GetStacking (LocalVariables|Get_DA_Item)) ; Stackable
    (for (_array_element _array_index) (Variables|Default|GetSlots) ; Search for similar
      (if (and (== (.DA_Item (Utilities|Struct|BreakInventorySlot _array_element)) (LocalVariables|Get_DA_Item)) (< (Math|Conversions|ToInteger(Byte) (.Quantity (Utilities|Struct|BreakInventorySlot _array_element))) (Math|Conversions|ToInteger(Byte) (Variables|/Script/SkyCraft.DA_Item|GetMaxStacking (LocalVariables|Get_DA_Item))))) ; Similar
        (if (> (+ (.Quantity (Utilities|Struct|BreakInventorySlot _array_element)) (LocalVariables|Get_LeftQuantity)) (Variables|/Script/SkyCraft.DA_Item|GetMaxStacking (LocalVariables|Get_DA_Item))) ; If stack overflow
          (LocalVariables|Set_LeftQuantity (- (+ (.Quantity (Utilities|Struct|BreakInventorySlot _array_element)) (LocalVariables|Get_LeftQuantity)) (Variables|/Script/SkyCraft.DA_Item|GetMaxStacking (LocalVariables|Get_DA_Item))))
          (CallFunction|MulticastSAE (Math|Conversions|ToByte(Integer) _array_index) (Utilities|Struct|MakeInventorySlot (.DA_Item (Utilities|Struct|BreakInventorySlot _array_element)) (Variables|/Script/SkyCraft.DA_Item|GetMaxStacking (LocalVariables|Get_DA_Item)) (.Properties (Utilities|Struct|BreakInventorySlot _array_element))))
          (else
            (CallFunction|MulticastSAE (Math|Conversions|ToByte(Integer) _array_index) (Utilities|Struct|MakeInventorySlot (.DA_Item (Utilities|Struct|BreakInventorySlot _array_element)) (+ (.Quantity (Utilities|Struct|BreakInventorySlot _array_element)) (LocalVariables|Get_LeftQuantity)) (.Properties (Utilities|Struct|BreakInventorySlot _array_element))))
            (return true (.quantity InventorySlot))))))
    (for (_array_element_2 _array_index_2) (Variables|Default|GetSlots) ; Search for empty
      (if (not (Utilities|IsValid (Utilities|Struct|BreakInventorySlot _array_element_2)))
        (CallFunction|MulticastSAE (Math|Conversions|ToByte(Integer) _array_index_2) (Utilities|Struct|MakeInventorySlot (.da_item InventorySlot) (LocalVariables|Get_LeftQuantity) (.properties InventorySlot)))
        (return true (.quantity InventorySlot))))
    (return (not (== (LocalVariables|Get_LeftQuantity) (.quantity InventorySlot))) (LocalVariables|Get_LeftQuantity))
    (else
      (for (_array_element_3 _array_index_3) (Variables|Default|GetSlots) ; Search for empty
        (if (not (Utilities|IsValid (Utilities|Struct|BreakInventorySlot _array_element_3)))
          (CallFunction|MulticastSAE (Math|Conversions|ToByte(Integer) _array_index_3) InventorySlot)
          (return true 0)))
      (return false (LocalVariables|Get_LeftQuantity)))))

(fn RemovefromInventory
  (params (RemoveIndex :type Byte) (RemoveQuantity :type Byte))
  (bind (_array_element _array_index) (Utilities|Array|ForEachLoopwithBreak (Variables|Default|GetSlots) :!label _label)
    (:LoopBody
      (if (== _array_index RemoveIndex)
        (if (> (- (.Quantity (Utilities|Struct|BreakInventorySlot _array_element)) RemoveQuantity) 0)
          (CallFunction|MulticastSAE RemoveIndex (Utilities|Struct|MakeInventorySlot (.DA_Item (Utilities|Struct|BreakInventorySlot _array_element)) (- (.Quantity (Utilities|Struct|BreakInventorySlot _array_element)) RemoveQuantity) (.Properties (Utilities|Struct|BreakInventorySlot _array_element))))
          (goto _label Break)
          (else
            (CallFunction|MulticastSAE RemoveIndex) ; empty
            (goto _label Break)))))))

(fn WastefromInventory
  (params (InventorySlot :type Inventory%20Slot%20Structure))
  (LocalVariables|SetHowManyNeed (Math|Conversions|ToInteger(Byte) (Utilities|Struct|BreakInventorySlot InventorySlot)))
  (bind (_array_element _array_index) (Utilities|Array|ForEachLoopwithBreak (Variables|Default|GetSlots) :!label _label)
    (:LoopBody
      (if (== (.DA_Item (Utilities|Struct|BreakInventorySlot _array_element)) (.da_item InventorySlot))
        (bind _output_get (LocalVariables|SetHowManyNeed (- (LocalVariables|GetHowManyNeed) (Math|Conversions|ToInteger(Byte) (.Quantity (Utilities|Struct|BreakInventorySlot _array_element))))))
        (if (== _output_get 0)
          (CallFunction|MulticastSAE (Math|Conversions|ToByte(Integer) _array_index))
          (goto _label Break)
          (elif (< _output_get 0)
            (CallFunction|MulticastSAE (Math|Conversions|ToByte(Integer) _array_index) (Utilities|Struct|MakeInventorySlot (.da_item (Utilities|Array|Get(acopy) (Variables|Default|GetSlots) _array_index)) (Math|Conversions|ToByte(Integer) (Math|Integer|Absolute(Integer) (LocalVariables|GetHowManyNeed))) (.properties (Utilities|Array|Get(acopy) (Variables|Default|GetSlots) _array_index))))
            (goto _label Break)))))))

(fn HMH
  (params (DA_Item :type DA%20Item%20Object%20Reference))
  (for _array_element (Variables|Default|GetSlots)
    (if (== (.DA_Item (Utilities|Struct|BreakInventorySlot _array_element)) DA_Item)
      (LocalVariables|Set_HMH (+ (.Quantity (Utilities|Struct|BreakInventorySlot _array_element)) (LocalVariables|Get_HMH)))))
  (return (LocalVariables|Get_HMH)))

(fn ServerSwap
  (params (SlotIndex :type Byte) (Dragged_Inventory :type Inventory%20Object%20Reference%20%28by%20ref%29) (Dragged_SlotIndex :type Byte))
  (bind _returnvalue (Math|Conversions|ToInteger(Byte) SlotIndex))
  (bind _slots (Variables|Default|GetSlots))
  (bind _output (Utilities|Array|Get(acopy) _slots _returnvalue))
  (bind _candropin (CallFunction|CanDropin Dragged_Inventory _output Dragged_SlotIndex))
  (if _candropin
    (LocalVariables|Set_Slot _output)
    (bind _output_get (LocalVariables|Set_DraggedSlot (Utilities|Array|Get(acopy) (Variables|Inventory_C|GetSlots Dragged_Inventory) (Math|Conversions|ToInteger(Byte) Dragged_SlotIndex))))
    (CallFunction|ServerSAE SlotIndex _output_get)
    (CallFunction|ServerSAE Dragged_Inventory Dragged_SlotIndex (LocalVariables|Get_Slot))
    (return)))

(fn CheckEmptySlots
  (for (_array_element _array_index) (Variables|Default|GetSlots)
    (if (not (Utilities|IsValid (Utilities|Struct|BreakInventorySlot _array_element)))
      (Utilities|Array|Add (LocalVariables|Get_EmptySlots) _array_index)))
  (return (LocalVariables|Get_EmptySlots)))

(fn ServerDropin
  (params (SlotIndex :type Byte) (Dragged_Inventory :type Inventory%20Object%20Reference) (Dragged_SlotIndex :type Byte) (Dragged_Quantity :type Byte))
  (bind _slots (Variables|Default|GetSlots))
  (bind _returnvalue (Math|Conversions|ToInteger(Byte) SlotIndex))
  (bind _returnvalue_2 (Math|Conversions|ToInteger(Byte) Dragged_SlotIndex))
  (bind _slots_2 (Variables|Inventory_C|GetSlots Dragged_Inventory))
  (bind _output (Utilities|Array|Get(acopy) _slots _returnvalue))
  (bind _output_2 (Utilities|Array|Get(acopy) _slots_2 _returnvalue_2))
  (if (!= self Dragged_Inventory) ; If inventory not self
    _
    (elif (!= Dragged_SlotIndex SlotIndex) ; If slot not self
      _
      (else
        (return))))
  (bind _candropin (CallFunction|CanDropin (Utilities|Array|Get(acopy) (Variables|Inventory_C|GetSlots Dragged_Inventory) (Math|Conversions|ToInteger(Byte) Dragged_SlotIndex)) SlotIndex))
  (if _candropin
    ;[1 1 1] Local Preperation
    (LocalVariables|Set_Slot_DA_Item (.da_item _output))
    (LocalVariables|Set_Slot_Quantity (.quantity _output))
    (LocalVariables|Set_Slot_Properties (.properties _output))
    (bind _output_get (LocalVariables|Set_DraggedSlot_Quantity (.quantity _output_2)))
    (LocalVariables|Set_DraggedLeft_Quantity (- _output_get Dragged_Quantity))
    (bind _output_get_2 (LocalVariables|Set_DraggedInventorySlot (Utilities|Struct|MakeInventorySlot (.da_item _output_2) Dragged_Quantity (.properties _output_2))))
    (LocalVariables|Set_Dragged_DA_Item (.da_item _output_get_2))
    (if (not (Utilities|IsValid (LocalVariables|Get_Slot_DA_Item))) ; If this slot is empty
      (CallFunction|ServerSAE SlotIndex (LocalVariables|Get_DraggedInventorySlot))
      (elif (== (LocalVariables|Get_Slot_DA_Item) (LocalVariables|Get_Dragged_DA_Item)) ; If the same type
        (if (Variables|/Script/SkyCraft.DA_Item|GetStacking (LocalVariables|Get_Slot_DA_Item)) ; If can stack
          (if (>= (LocalVariables|Get_Slot_Quantity) (Variables|/Script/SkyCraft.DA_Item|GetMaxStacking (LocalVariables|Get_Slot_DA_Item))) ; If full stack
            (CallFunction|ServerSwap SlotIndex Dragged_Inventory Dragged_SlotIndex :!label _label)
            (return)
            (elif (< (+ (LocalVariables|Get_Slot_Quantity) Dragged_Quantity) (Variables|/Script/SkyCraft.DA_Item|GetMaxStacking (LocalVariables|Get_Slot_DA_Item))) ; If added stack not overflow
              (CallFunction|ServerSAE SlotIndex (Utilities|Struct|MakeInventorySlot (LocalVariables|Get_Slot_DA_Item) (+ (LocalVariables|Get_Slot_Quantity) Dragged_Quantity) (LocalVariables|Get_Slot_Properties)))
              (else
                (if (> (+ (- (+ (LocalVariables|Get_Slot_Quantity) Dragged_Quantity) (Variables|/Script/SkyCraft.DA_Item|GetMaxStacking (LocalVariables|Get_Slot_DA_Item))) (LocalVariables|Get_DraggedLeft_Quantity)) 0) ; If leftover > 0
                  (CallFunction|ServerSAE Dragged_Inventory Dragged_SlotIndex (Utilities|Struct|MakeInventorySlot (.da_item (LocalVariables|Get_DraggedInventorySlot)) (+ (- (+ (LocalVariables|Get_Slot_Quantity) Dragged_Quantity) (Variables|/Script/SkyCraft.DA_Item|GetMaxStacking (LocalVariables|Get_Slot_DA_Item))) (LocalVariables|Get_DraggedLeft_Quantity)) (.properties (LocalVariables|Get_DraggedInventorySlot))))
                  (else
                    (CallFunction|ServerSAE Dragged_Inventory Dragged_SlotIndex) ; empty
                  ))
                (CallFunction|ServerSAE SlotIndex (Utilities|Struct|MakeInventorySlot (LocalVariables|Get_Slot_DA_Item) (Variables|/Script/SkyCraft.DA_Item|GetMaxStacking (LocalVariables|Get_Slot_DA_Item)) (LocalVariables|Get_Slot_Properties)))
                (return))))
          (else
            (goto _label)))
        (else
          (goto _label))))
    (if (> (LocalVariables|Get_DraggedLeft_Quantity) 0) ; If left in dragged slot
      (CallFunction|ServerSAE Dragged_Inventory Dragged_SlotIndex (Utilities|Struct|MakeInventorySlot (.da_item (LocalVariables|Get_DraggedInventorySlot)) (LocalVariables|Get_DraggedLeft_Quantity) (.properties (LocalVariables|Get_DraggedInventorySlot))))
      (else
        (CallFunction|ServerSAE Dragged_Inventory Dragged_SlotIndex) ; empty
      ))
    (return)
    (else
      (return))))

(fn CanDropin
  (params (InventorySlot :type Inventory%20Slot%20Structure) (DropIn_SlotIndex :type Byte))
  (return true))

(fn GetInventorySlotIndex
  (return 0))

(fn SetSlotDarken
  (params (Darken :type Boolean))
  (return false))

(fn SetSlotHighlight
  (params (Hovered :type Boolean))
  (return false))

(fn UpdateInventorySlot
  (return false))