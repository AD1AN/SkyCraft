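; Blueprint function library of shared helpers for essence math, custom-settings saves and small actor, vector, array and property utilities.
; Essence helpers treat Red, Green and Blue amounts as a resource, with normalized RGB conversion and an iterative subtraction that spreads cost evenly, dropping depleted colors.
; LoadCustomSettings guarantees a valid selected character bio, repairing the index or calling CreateRandomCharacter to generate and save one, then returns the reloaded save.
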(fn GetRootActor
  (params (StartActor :type Actor%20Object%20Reference))
  (bind _output_get (LocalVariables|SetCurrentParent StartActor))
  (LocalVariables|SetLastValidParent _output_get)
  (while (Utilities|IsValid (LocalVariables|GetCurrentParent))
    (bind _output_get_2 (LocalVariables|SetCurrentParent (Actor|GetAttachParentActor (LocalVariables|GetCurrentParent))))
    (Utilities|IsValid _output_get_2
      (:Is%20Valid
        (LocalVariables|SetLastValidParent (LocalVariables|GetCurrentParent)))))
  (return (LocalVariables|GetLastValidParent)))

(fn AddEssence
  (params (1 :type S%20Essence%20Structure) (2 :type S%20Essence%20Structure))
  (bind (_red _green _blue) (Utilities|Struct|BreakS_Essence 1))
  (bind (_red_2 _green_2 _blue_2) (Utilities|Struct|BreakS_Essence 2))
  (return (Utilities|Struct|MakeS_Essence (+ _red _red_2) (+ _green _green_2) (+ _blue _blue_2))))

(fn SubtractEssence
  (params (1 :type S%20Essence%20Structure) (2 :type S%20Essence%20Structure))
  (bind (_red _green _blue) (Utilities|Struct|BreakS_Essence 1))
  (bind (_red_2 _green_2 _blue_2) (Utilities|Struct|BreakS_Essence 2))
  (return (Utilities|Struct|MakeS_Essence (- _red _red_2) (- _green _green_2) (- _blue _blue_2))))

(fn EssenceMax
  (params (Essence :type S%20Essence%20Structure))
  (return (Math|Conversions|ToFloat(Integer) (Math|Integer|Max(Integer) (.red Essence) (.green Essence) (.blue Essence)))))

(fn EssenceRGB
  (params (Essence :type S%20Essence%20Structure))
  (return (Math|Float|MapRangeClamped (Math|Conversions|ToFloat(Integer) (.red Essence)) 0.0 (CallFunction|EssenceMax Essence) 0.0 1.0) (Math|Float|MapRangeClamped (Math|Conversions|ToFloat(Integer) (.green Essence)) 0.0 (CallFunction|EssenceMax Essence) 0.0 1.0) (Math|Float|MapRangeClamped (Math|Conversions|ToFloat(Integer) (.blue Essence)) 0.0 (CallFunction|EssenceMax Essence) 0.0 1.0)))

(fn Int->Stream->Int
  (params (InitialSeed :type Integer))
  (return (Class|KismetMathLibrary|RandomIntegerfromStream 2147483647 (Math|Random|MakeRandomStream InitialSeed))))

(fn UniformMinusEssence
  (params (Essence :type S%20Essence%20Structure) (Minus :type Integer))
  (LocalVariables|SetTempEssence Essence)
  (LocalVariables|SetMinusLeft Minus)
  (while true
    (LocalVariables|SetUniformConsume (Math|Integer|SelectInt (/ (LocalVariables|GetMinusLeft) (Utilities|Array|Length (LocalVariables|GetEssenceColors))) 1 (> (/ (LocalVariables|GetMinusLeft) (Utilities|Array|Length (LocalVariables|GetEssenceColors))) 0)))
    (for _array_element (LocalVariables|GetEssenceColors)
      (bind _output_get (LocalVariables|SetElemColor _array_element))
      (LocalVariables|SetElemLeft (- (Utilities|Select :Index (- _output_get 1) :Option%200 (.red (LocalVariables|GetTempEssence)) :Option%201 (.green (LocalVariables|GetTempEssence)) :Option%202 (.blue (LocalVariables|GetTempEssence))) (LocalVariables|GetUniformConsume)))
      (if (>= (- (Utilities|Select :Index (- _output_get 1) :Option%200 (.red (LocalVariables|GetTempEssence)) :Option%201 (.green (LocalVariables|GetTempEssence)) :Option%202 (.blue (LocalVariables|GetTempEssence))) (LocalVariables|GetUniformConsume)) 0)
        (LocalVariables|SetMinusLeft (- (LocalVariables|GetMinusLeft) (LocalVariables|GetUniformConsume)))
        (if (== (LocalVariables|GetElemLeft) 0)
          (Utilities|Array|Add (LocalVariables|GetColorRemove) (LocalVariables|GetElemColor)))
        (else
          (LocalVariables|SetMinusLeft (- (LocalVariables|GetMinusLeft) (Utilities|Select :Index (- _output_get 1) :Option%200 (.red (LocalVariables|GetTempEssence)) :Option%201 (.green (LocalVariables|GetTempEssence)) :Option%202 (.blue (LocalVariables|GetTempEssence)))))
          (LocalVariables|SetElemLeft 0)
          (Utilities|Array|Add (LocalVariables|GetColorRemove) (LocalVariables|GetElemColor))))
      (switch int (- (LocalVariables|GetElemColor) 1)
        (:0
          (Utilities|Struct|SetmembersinS_Essence (LocalVariables|GetTempEssence) (LocalVariables|GetElemLeft)))
        (:1
          (Utilities|Struct|SetmembersinS_Essence (LocalVariables|GetTempEssence) (LocalVariables|GetElemLeft)))
        (:2
          (Utilities|Struct|SetmembersinS_Essence (LocalVariables|GetTempEssence) (LocalVariables|GetElemLeft))))
      (if (or (<= (LocalVariables|GetMinusLeft) 0) (== (Utilities|Array|Length (LocalVariables|GetEssenceColors)) 0))
        (return (LocalVariables|GetTempEssence))))
    (for _array_element_2 (LocalVariables|GetColorRemove)
      (Utilities|Array|RemoveItem (LocalVariables|GetEssenceColors) _array_element_2))
    (if (or (<= (LocalVariables|GetMinusLeft) 0) (== (Utilities|Array|Length (LocalVariables|GetEssenceColors)) 0))
      (return (LocalVariables|GetTempEssence)))))

(fn EssenceTotal
  (params (Essence :type S%20Essence%20Structure))
  (return (+ (.red Essence) (.green Essence) (.blue Essence))))

(fn DistanceMeters
  (params (A :type Actor%20Object%20Reference) (B :type Actor%20Object%20Reference))
  (return (Math|Float|Truncate (/ (Math|Vector|Distance(Vector) (Transformation|GetActorLocation A) (Transformation|GetActorLocation B)) 1e+02))))

(fn EquipmentType
  (params (EQIndex :type Integer))
  (return (Utilities|Select :Index EQIndex :Option%200 "EQHead" :Option%201 "EQChest" :Option%202 "EQHands" :Option%203 "EQLegs" :Option%204 "EQFeet")))

(fn FindProperty
  (params (FindProperty :type DA%20Item%20Property%20Object%20Reference) (SearchInProperties :type Array%20of%20Item%20Property%20Structures))
  (bind (_array_element _array_index) (Utilities|Array|ForEachLoopwithBreak SearchInProperties)
    (:LoopBody
      (if (== (Utilities|Struct|BreakItemProperty _array_element) FindProperty)
        (return true _array_element _array_index)))
    (:Completed
      (return false "" 0))))

(fn A1PrintError
  (params (Message :type String))
  (Development|PrintString 0 Message true true "(R=1.000000,G=0.000000,B=0.016666,A=1.000000)" 15.0))

(fn CreateRandomCharacter
  (params (SSG_CustomSettings :type Custom%20Settings%20Save%20Object%20Reference))
  (bind _returnvalue (Math|Random|RandomInteger 9))
  (bind _returnvalue_2 (Math|Random|RandomBool))
  (bind _returnvalue_3 (Utilities|Array|Add (Variables|/Game/Blueprints/CustomSettingsSave.CustomSettingsSave_C|GetCharactersBio SSG_CustomSettings) (Utilities|Struct|MakeS_CharacterBio (select _returnvalue_2 (Utilities|Select :Index _returnvalue :Option%200 "Lukas" :Option%201 "Wigmar" :Option%202 "Tullus" :Option%203 "Ellis" :Option%204 "Opiter" :Option%205 "Tertius" :Option%206 "Manius" :Option%207 "Nofri" :Option%208 "Lambertus" :Option%209 "Binet") (Utilities|Select :Index _returnvalue :Option%200 "Mary" :Option%201 "Sittia" :Option%202 "Nora" :Option%203 "Lorraine" :Option%204 "Eva" :Option%205 "Eileen" :Option%206 "Amelina" :Option%207 "Silia" :Option%208 "Plinia" :Option%209 "Vanessa")) _returnvalue_2 "None" (Class|KismetMathLibrary|HSVtoRGB (Math|Random|RandomFloatinRange 0.0 3.6e+02) (Math|Random|RandomFloatinRange 0.0 1.0) (Math|Random|RandomFloatinRange 0.1 0.55) 1.0) (Class|KismetMathLibrary|HSVtoRGB (Math|Random|RandomFloatinRange 0.0 3.6e+02) (Math|Random|RandomFloatinRange 0.0 1.0) (Math|Random|RandomFloatinRange 0.1 0.55) 1.0) (Math|Random|RandomFloatinRange 0.9 1.0) (Math|DateTime|Now))))
  (Default|SetSelectedCharacterBioIndex SSG_CustomSettings _returnvalue_3)
  (SaveGame|SaveGametoSlot SSG_CustomSettings "CustomSettings")
  (return))

(fn LoadCustomSettings
  (Utilities|FlowControl|Sequence
    (:then_0
      (bind _returnvalue (SaveGame|DoesSaveGameExist "CustomSettings"))
      (if _returnvalue
        (bind _returnvalue_2 (SaveGame|LoadGamefromSlot "CustomSettings"))
        (bind _customsettingssave (Class|BPISSG|GetCustomSettingsSave(Message) _returnvalue_2))
        (if (not (Utilities|Array|IsValidIndex (Variables|/Game/Blueprints/CustomSettingsSave.CustomSettingsSave_C|GetCharactersBio _customsettingssave) (Default|GetSelectedCharacterBioIndex _customsettingssave)))
          (if (Utilities|Array|IsEmpty (Variables|/Game/Blueprints/CustomSettingsSave.CustomSettingsSave_C|GetCharactersBio _customsettingssave))
            (CallFunction|CreateRandomCharacter _customsettingssave)
            (else
              (Default|SetSelectedCharacterBioIndex _customsettingssave (Utilities|Array|LastIndex (Variables|/Game/Blueprints/CustomSettingsSave.CustomSettingsSave_C|GetCharactersBio _customsettingssave)))
              (SaveGame|SaveGametoSlot _customsettingssave "CustomSettings"))))
        (else
          (bind _returnvalue_3 (SaveGame|CreateSaveGameObject "/Game/Blueprints/CustomSettingsSave.CustomSettingsSave_C"))
          (CallFunction|CreateRandomCharacter _returnvalue_3))))
    (:then_1
      (bind _returnvalue_4 (SaveGame|LoadGamefromSlot "CustomSettings"))
      (bind _customsettingssave_2 (Class|BPISSG|GetCustomSettingsSave(Message) _returnvalue_4))
      (return _customsettingssave_2))))

(fn VectorSignInvert
  (params (InVector :type Vector) (InvertX :type Boolean) (InvertY :type Boolean) (InvertZ :type Boolean))
  (bind (_x _y _z) (Class|KismetMathLibrary|BreakVector3f InVector))
  (return (Math|Vector|MakeVector (Math|Float|SelectFloat (* _x -1.0) _x InvertX) (Math|Float|SelectFloat (* _y -1.0) _y InvertY) (Math|Float|SelectFloat (* _z -1.0) _z InvertZ))))

(fn CombineArrays
  (params (From :type Array%20of%20Object%20Object%20References) (To :type Array%20of%20Object%20Object%20References))
  (for _array_element From
    (Utilities|Array|Add To _array_element)))