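; Test death-essence actor that runs a Niagara effect sourced from a character's skeletal mesh and attracted toward a consuming actor.
; On BeginPlay it overrides the system's SkeletalMesh user variable with the Character's mesh and activates the effect.
; While ConsumeActor is valid, Tick feeds its location, converted to this actor's local space, into AttractorPosition.
; System completion only prints a debug string.
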(event OnSystemFinished(Niagara)
  (params (PSystem :type Niagara%20Component%20Object%20Reference))
  (Development|PrintString "Hello"))

(event EventTick
  (params (DeltaSeconds :type Float%20%28single-precision%29))
  (bind _consumeactor (Variables|Default|GetConsumeActor))
  (Utilities|IsValid _consumeactor
    (:Is%20Valid
      (Niagara|SetNiagaraVariable(Vector3) (Variables|Default|GetNiagara) "AttractorPosition" (Math|Transform|InverseTransformLocation (Transformation|GetActorTransform) (Transformation|GetActorLocation _consumeactor))))))

(event EventBeginPlay
  (Class|NiagaraFunctionLibrary|OverrideSystemUserVariableSkeletalMeshComponent (Variables|Default|GetNiagara) "SkeletalMesh" (Variables|/Script/Engine.Character|GetMesh (Variables|Default|GetCharacter)))
  (Components|Activation|SetActive (Variables|Default|GetNiagara) true false))

(fn ConstructionScript)