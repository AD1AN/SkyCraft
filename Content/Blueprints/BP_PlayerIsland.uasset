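; BP_PlayerIsland is a player's moving island: steered by direction, speed and altitude, powered by Essence and restored from saves.
; The server stops it on island collisions, drops it to minimum speed on Essence deficit, and destroys its buildings when it loses its crystal.
; Timed resizes trade Essence, with a space check before expanding.
; Multicasts and RepNotifies drive rumble, shake and Niagara effects, while crystal state selects the menu.
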(event OnComponentBeginOverlap(IslandCollision)
  (params (OverlappedComponent :type Primitive%20Component%20Object%20Reference) (OtherActor :type Actor%20Object%20Reference) (OtherComp :type Primitive%20Component%20Object%20Reference) (OtherBodyIndex :type Integer) (bFromSweep :type Boolean) (SweepResult :type Hit%20Result%20Structure%20%28by%20ref%29))
  (Utilities|IsValid OtherActor
    (:Is%20Valid
      (if (and (!= OtherActor self) (Class|GameplayStatics|ObjectIsA OtherActor "/Script/SkyCraft.Island"))
        (CallFunction|MulticastFXIslandCollide)
        (CallFunction|ServerStopIsland)))))

(event Custom|StartResizeIsland
  (params (NewSize :type Integer) (PlayerInstigator :type BP%20PSS%20Object%20Reference))
  (bind _returnvalue (Class|PlayerIsland|GetIslandSizeNum))
  (bind _expandcost (Variables|ConfigVariables|GetExpandCost))
  (bind _returnvalue_2 (- NewSize _returnvalue))
  (bind _returnvalue_3 (* _returnvalue_2 _expandcost))
  (if (and (!= NewSize (Class|PlayerIsland|GetIslandSizeNum)) (not (Variables|Default|GetResizing)))
    (if (> NewSize (Class|PlayerIsland|GetIslandSizeNum))
      (if (CallFunction|CheckEnoughEssence _returnvalue_3)
        (bind _valid (CallFunction|CheckResizeSpace NewSize))
        (if _valid
          (Class|PlayerIsland|SetEssence (- (Class|PlayerIsland|GetEssence) _returnvalue_3))
          (Variables|Default|SetResizeNewSize NewSize :!label _label)
          (CallFunction|ServerStopIsland)
          (Variables|Default|SetResizing true)
          (CallFunction|MulticastFXStartResize)
          (Utilities|Time|SetTimerbyEvent (delegate Custom|FinishResize) 5.0)
          (else
            (Class|PSS|ClientActionWarning PlayerInstigator "Another island is blocking your island's expansion."))))
      (else
        (Class|PlayerIsland|SetEssence (+ (* (- (Class|PlayerIsland|GetIslandSizeNum) NewSize) (Variables|ConfigVariables|GetShrinkCost)) (Class|PlayerIsland|GetEssence)))
        (goto _label)))))

(event Custom|FinishResize
  (Class|PlayerIsland|SetIslandSize (Math|Float|MapRangeClamped (Math|Conversions|ToFloat(Integer) (Variables|Default|GetResizeNewSize)) 1.0 1e+02 0.0 1.0))
  (Variables|Default|SetResizing false)
  (CallFunction|MulticastFXCompleteResize))

(event Custom|Server_StopIsland
  (CallFunction|MulticastStopIsland (Variables|Default|GetPreviousLocation)))

(event Custom|MulticastFX_IslandCollide
  (Audio|SpawnSoundAttached "/Game/Audio/SFX/IslandCollide.IslandCollide" (Variables|Transformation|GetRootComponent) "None" "0, 0, 0" "0, 0, 0" "KeepRelativeOffset" false (Math|Float|MapRangeClamped (Variables|Default|GetCurrentSpeed) 0.0 (/ (Variables|Default|GetTargetSpeedMax) 2.5) 0.05 1.0) 1.0 0.0 "/Game/Audio/WholeIslandAttenuation.WholeIslandAttenuation" 0)
  (Camera|PlayWorldCameraShake "/Game/Blueprints/CameraShake/CS_IslandCollide.CS_IslandCollide_C" (Transformation|GetActorLocation) 1e+04 5e+03))

(event Custom|MulticastFX_CompleteResize
  (bind _shaperadius (Variables|Default|GetShapeRadius))
  (bind _cs_rumble (Variables|Default|GetCS_Rumble))
  (bind _ns_islandrumble (Variables|Default|GetNS_IslandRumble))
  (bind _returnvalue (+ _shaperadius 8e+03))
  (if (not (Networking|IsDedicatedServer))
    (Class|AudioParameterControllerInterface|SetTriggerParameter (Variables|Default|GetAudioRumble) "CompleteResize")
    (Camera|PlayWorldCameraShake "/Game/Blueprints/CameraShake/CS_BigImpact.CS_BigImpact_C" (Transformation|GetActorLocation) _returnvalue _returnvalue)
    (Utilities|FlowControl|Sequence
      (:then_0
        (Utilities|IsValid _cs_rumble
          (:Is%20Valid
            (CameraShake|StopAllCameraShakes _cs_rumble false)
            (Components|DestroyComponent (Variables|Default|GetCS_Rumble)))))
      (:then_1
        (Utilities|IsValid _ns_islandrumble
          (:Is%20Valid
            (Components|Activation|SetActive _ns_islandrumble false false)))))))

(event Custom|MulticastFX_StartResize
  (if (not (Networking|IsDedicatedServer))
    (Audio|Components|Audio|Play (Variables|Default|GetAudioRumble) 0.0)
    (bind _returnvalue (AddComponent|AddCameraShakeSourceComponent false))
    (bind _output_get (Variables|Default|SetCS_Rumble _returnvalue))
    (bind _output_get_2 (Variables|/Script/Engine.CameraShakeSourceComponent|SetInnerAttenuationRadius _output_get (+ (Variables|Default|GetShapeRadius) 8e+03)))
    (Variables|/Script/Engine.CameraShakeSourceComponent|SetOuterAttenuationRadius _output_get _output_get_2)
    (bind _returnvalue_2 (Niagara|SpawnSystemAttached "/Game/Niagara/NS_IslandRumble.NS_IslandRumble" (Variables|Transformation|GetRootComponent) "None" "0, 0, 0" "0, 0, 0" "KeepRelativeOffset" true))
    (bind _output_get_3 (Variables|Default|SetNS_IslandRumble _returnvalue_2))
    (Class|NiagaraDataInterfaceArrayFunctionLibrary|SetNiagaraArrayPosition _output_get_3 "Vertices" (.topvertices (Variables|Default|GetID)))
    (Niagara|SetNiagaraVariable(Float) _output_get_3 "IslandSizeRatio" (Variables|Default|GetIslandSize))))

(event Custom|Multicast_StopIsland
  (params (ServerLocation :type Vector))
  (Transformation|SetActorLocation ServerLocation false true) ; Teleport: True
  (Class|PlayerIsland|SetStopIsland true)
  (Variables|Default|SetCurrentSpeed 0.0)
  (Class|PlayerIsland|SetAltitudeDirection 0.0)
  (Class|PlayerIsland|SetTargetAltitude (.z (Variables|Default|GetPreviousLocation)))
  (Audio|SpawnSoundAttached "/Game/Audio/SFX/IslandStop.IslandStop" (Variables|Transformation|GetRootComponent) "None" "0, 0, 0" "0, 0, 0" "KeepRelativeOffset" false 1.0 1.0 0.0 "/Game/Audio/WholeIslandAttenuation.WholeIslandAttenuation" 0))

(event Custom|OnEssence_Event
  (CallFunction|CheckEssenceDeficit))

(event Custom|OnDie_Event
  (Class|PlayerIsland|SetIsCrystal false))

(event Custom|OnIslandSize_Event
  (bind _shaperadius (Variables|Default|GetShapeRadius))
  (Components|Capsule|SetCapsuleRadius (Variables|Default|GetIslandCollision) (Variables|Default|GetShapeRadius) true)
  (Components|Capsule|SetCapsuleHalfHeight (Variables|Default|GetIslandCollision) (* 1.25 _shaperadius) true)
  (Transformation|SetRelativeLocation (Variables|Default|GetIslandCollision) (Math|Vector|MakeVector 0.0 0.0 (* -0.2 _shaperadius)) false true)
  (Niagara|SetNiagaraVariable(Float) (Variables|Default|GetNS_Direction) "Radius" (Variables|Default|GetShapeRadius))
  (Niagara|SetNiagaraVariable(Float) (Variables|Default|GetNS_Direction) "IslandSizeRatio" (Variables|Default|GetIslandSize))
  (Niagara|SetNiagaraVariable(Float) (Variables|Default|GetNiagaraWind) "Radius" (Variables|Default|GetShapeRadius))
  (Niagara|SetNiagaraVariable(Float) (Variables|Default|GetNiagaraWind) "IslandSizeRatio" (Variables|Default|GetIslandSize))
  (Utilities|Struct|SetmembersinSoundAttenuationSettings (Variables|/Script/Engine.AudioComponent|GetAttenuationOverrides (Variables|Default|GetAudioRumble)) (Math|Vector|MakeVector (+ (Variables|Default|GetShapeRadius) 5e+03) 0.0 0.0)))

(event Custom|Multicast_UnstopIsland
  (Class|PlayerIsland|SetStopIsland false))

(event Custom|Server_UnstopIsland
  (if (> (Class|PlayerIsland|GetEssence) 0)
    (CallFunction|MulticastUnstopIsland)))

(event EventBeginPlay
  (bind _returnvalue (Math|Random|RandomRotator false))
  (bind _targetspeedmin (Variables|Default|GetTargetSpeedMin))
  (bind _ss_playerisland (Variables|Default|GetSS_PlayerIsland))
  (bind (_archonsteamid _targetdirection _targetaltitude _targetspeed _stopisland _essence _astralons) (Utilities|Struct|BreakSS_PlayerIsland _ss_playerisland))
  (bind _returnvalue_2 (Math|Vector|GetForwardVector (Math|Rotator|MakeRotator 0.0 0.0 (.yaw _returnvalue))))
  (bind _returnvalue_3 (Class|AdianFL|ToQuantizeNormal(Vector) _returnvalue_2))
  (Utilities|FlowControl|Sequence
    (:then_0
      (Networking|SwitchHasAuthority
        (:Authority
          (Collision|SetCollisionEnabled (Variables|Default|GetIslandCollision) "QueryOnly")
          (bind _asbp_gms (Utilities|Casting|CastToBP_GMS (Game|GetGameMode)))
          (Variables|LocalVariables|SetBP_GMS _asbp_gms)
          (EventDispatchers|BindEventtoOnDie (Variables|/Script/SkyCraft.IslandCrystal|GetEntityComponent (Variables|Default|GetIslandCrystal)) (delegate Custom|OnDie_Event))
          (EventDispatchers|BindEventtoOnEssence (delegate Custom|OnEssence_Event))
          (Class|PlayerIsland|SetTargetAltitude (.z (Transformation|GetActorLocation)))
          (if (Variables|Default|GetbLoadFromSave)
            (Class|PlayerIsland|AuthSetArchonSteamID _archonsteamid)
            (Class|PlayerIsland|SetTargetDirection _targetdirection)
            (Class|PlayerIsland|SetTargetAltitude _targetaltitude)
            (Class|PlayerIsland|SetTargetSpeed _targetspeed)
            (Class|PlayerIsland|SetStopIsland _stopisland)
            (Class|PlayerIsland|SetEssence _essence)
            (Variables|Default|SetSS_Astralons _astralons)
            (else
              (Class|PlayerIsland|SetTargetDirection _returnvalue_3)
              (Variables|Default|SetCurrentDirection _returnvalue_3)
              (Class|PlayerIsland|SetTargetSpeed _targetspeedmin)
              (Variables|Default|SetCurrentSpeed _targetspeedmin))))))
    (:then_1
      (EventDispatchers|AssignOnIslandSize (delegate Custom|OnIslandSize_Event))
      (CallFunction|OnIslandSizeEvent)
      (Variables|Default|SetIslandStarted true))))

(event EventOnRepPawnIslandControl
  (bind _asbp_pawn_island_control (Utilities|Casting|CastToBP_PawnIslandControl (Variables|Default|GetPawnIslandControl)))
  (Variables|Default|SetBP_PawnIslandControl _asbp_pawn_island_control))

(event EventOnIslandShrink
  (for _array_element (Variables|Default|GetBuildings)
    (if (Class|AdianFL|ActorHasSkyTag _array_element "/Game/DataAssets/SkyTag/ST_Building_Foundation.ST_Building_Foundation")
      (bind _asbm_foundation (Utilities|Casting|CastToBM_Foundation _array_element))
      (bind _valid (Default|GridTraces _asbm_foundation))
      (if (not _valid)
        (Class|BM|Dismantle _asbm_foundation)))))

(event EventOnRepBIsCrystal
  (bind _returnvalue (Transformation|GetActorLocation))
  (bind _returnvalue_2 (Transformation|GetActorLocation))
  (bind _shaperadius (Variables|Default|GetShapeRadius))
  (bind _shaperadius_2 (Variables|Default|GetShapeRadius))
  (bind _buildings (Variables|Default|GetBuildings))
  (bind _returnvalue_3 (+ _shaperadius_2 8e+03))
  (bind _returnvalue_4 (+ _shaperadius 8e+03))
  (if (Variables|Default|GetIslandStarted)
    (|CallParentFunction)
    (Utilities|FlowControl|Sequence
      (:then_0
        (if (Variables|Default|GetbIsCrystal)
          (Variables|Default|SetbIslandCanSave true)
          (if (not (Networking|IsDedicatedServer))
            (bind _returnvalue_5 (Niagara|SpawnSystemAttached "/Game/Niagara/NS_IslandGroundBurst.NS_IslandGroundBurst" (Variables|Transformation|GetRootComponent) "None" "0, 0, 0" "0, 0, 0" "KeepRelativeOffset" true))
            (Class|NiagaraDataInterfaceArrayFunctionLibrary|SetNiagaraArrayPosition _returnvalue_5 "Vertices" (.topvertices (Variables|Default|GetID)))
            (Niagara|SetNiagaraVariable(Float) _returnvalue_5 "IslandSizeRatio" (Variables|Default|GetIslandSize))
            (Audio|SpawnSoundatLocation "/Game/Audio/SFX/Death.Death" _returnvalue "0, 0, 0" 3.0 0.75 0.0 "/Game/Audio/WholeIslandAttenuation.WholeIslandAttenuation" 0)
            (Audio|SpawnSoundatLocation "/Game/Audio/SFX/IslandRumbleCompleteResize.IslandRumbleCompleteResize" _returnvalue "0, 0, 0" 2.0 0.8 0.0 "/Game/Audio/WholeIslandAttenuation.WholeIslandAttenuation" 0)
            (Camera|PlayWorldCameraShake "/Game/Blueprints/CameraShake/CS_BigImpact.CS_BigImpact_C" (Transformation|GetActorLocation) _returnvalue_3 _returnvalue_3))
          (else
            (Audio|SpawnSoundatLocation "/Game/Audio/SFX/Death.Death" _returnvalue_2 "0, 0, 0" 3.0 0.75 0.0 "/Game/Audio/WholeIslandAttenuation.WholeIslandAttenuation" 0)
            (Audio|SpawnSoundatLocation "/Game/Audio/SFX/IslandRumbleCompleteResize.IslandRumbleCompleteResize" _returnvalue_2 "0, 0, 0" 2.0 0.8 0.0 "/Game/Audio/WholeIslandAttenuation.WholeIslandAttenuation" 0)
            (Camera|PlayWorldCameraShake "/Game/Blueprints/CameraShake/CS_BigImpact.CS_BigImpact_C" (Transformation|GetActorLocation) _returnvalue_4 _returnvalue_4)
            (Networking|SwitchHasAuthority
              (:Authority
                (Actor|DestroyActor _buildings)
                (Utilities|Array|Clear _buildings)
                (CallFunction|ServerStopIsland))))))
      (:then_1
        (Networking|SwitchHasAuthority
          (:Authority
            (Variables|Default|SetEssenceDeficit false)))))))

(fn ConstructionScript)

(fn CreateMenu
  (params (Pawn :type Pawn%20Object%20Reference) (BP_PSS :type BP%20PSS%20Object%20Reference))
  (if (Variables|Default|GetbIsCrystal)
    (Utilities|IsValid (Variables|LocalVariables|GetCWS_Crystal_PlayerIsland)
      (:Is%20Valid
        _)
      (:Is%20Not%20Valid
        (bind _returnvalue (UserInterface|CreateWidget "/Game/Widgets/CWS/CWS_PlayerIsland_Crystal.CWS_PlayerIsland_Crystal_C" 0 self))
        (Variables|LocalVariables|SetCWS_Crystal_PlayerIsland _returnvalue)))
    (Default|ShowMenu (Variables|LocalVariables|GetCWS_Crystal_PlayerIsland) (EventDispatchers|CreateEvent :!event ShowCompleted))
    (UserInterface|Viewport|AddtoViewport (Variables|LocalVariables|GetCWS_Crystal_PlayerIsland) 20)
    (Default|AddCWS BP_PSS (Variables|LocalVariables|GetCWS_Crystal_PlayerIsland) true true true "NewEnumerator2")
    (Default|SetMouseto BP_PSS 2.0 2.0)
    (else
      (Utilities|IsValid (Variables|LocalVariables|GetCWS_NonCrystal_PlayerIsland)
        (:Is%20Valid
          _)
        (:Is%20Not%20Valid
          (bind _returnvalue_2 (UserInterface|CreateWidget "/Game/Widgets/CWS/CWS_PlayerIsland_NonCrystal.CWS_PlayerIsland_NonCrystal_C" 0 self))
          (Variables|LocalVariables|SetCWS_NonCrystal_PlayerIsland _returnvalue_2)))
      (Default|ShowMenu (Variables|LocalVariables|GetCWS_NonCrystal_PlayerIsland))
      (UserInterface|Viewport|AddtoViewport (Variables|LocalVariables|GetCWS_NonCrystal_PlayerIsland) 20)
      (Default|AddCWS BP_PSS (Variables|LocalVariables|GetCWS_NonCrystal_PlayerIsland) true true true "NewEnumerator2")
      (Default|SetMouseto BP_PSS 2.0 2.0))))

(fn ShowCompleted)

(fn CheckEnoughEssence
  (params (RequireEssence :type Integer))
  (return (> (Class|PlayerIsland|GetEssence) RequireEssence)))

(fn CheckEssenceDeficit
  (if (< (Class|PlayerIsland|GetEssence) 1000)
    (if (not (Variables|Default|GetEssenceDeficit))
      (Variables|Default|SetEssenceDeficit true)
      (Class|PlayerIsland|SetTargetSpeed (Variables|Default|GetTargetSpeedMin))
      (Default|CallOnEssenceDeficit :!label _label))
    (elif (Variables|Default|GetEssenceDeficit)
      (Variables|Default|SetEssenceDeficit false)
      (goto _label))))

(fn OnRepBurnEssence
  (Default|CallOnBurnEssence))

(fn OnRepEssenceDeficit
  (Default|CallOnEssenceDeficit))

(fn OnRepCollapseTime
  (if (not (== (Variables|Default|GetCollapseTime) 0))
    (Default|CallOnCollapseTime)))

(fn OnRepCollapsing
  (Default|CallOnCollapsing)
  (Variables|Default|SetCollapseTime 0)
  (if (not (Networking|IsDedicatedServer))
    (if (Variables|Default|GetCollapsing)
      (Audio|Components|Audio|Play (Variables|Default|GetAudioRumble) 0.0)
      (Utilities|IsValid (Variables|Default|GetCS_Rumble)
        (:Is%20Valid
          (CameraShake|StopAllCameraShakes (Variables|Default|GetCS_Rumble) false)
          (Components|DestroyComponent (Variables|Default|GetCS_Rumble)))
        (:Is%20Not%20Valid
          _))
      (bind _returnvalue (AddComponent|AddCameraShakeSourceComponent false))
      (bind _output_get (Variables|Default|SetCS_Rumble _returnvalue))
      (bind _output_get_2 (Variables|/Script/Engine.CameraShakeSourceComponent|SetInnerAttenuationRadius _output_get (+ (Variables|Default|GetShapeRadius) 8e+03)))
      (Variables|/Script/Engine.CameraShakeSourceComponent|SetOuterAttenuationRadius _output_get _output_get_2)
      (Utilities|IsValid (Variables|Default|GetNS_IslandRumble)
        (:Is%20Valid
          (Class|AdianFL|ForceDestroyComponent (Variables|Default|GetNS_IslandRumble)))
        (:Is%20Not%20Valid
          _))
      (bind _returnvalue_2 (Niagara|SpawnSystemAttached "/Game/Niagara/NS_IslandRumble.NS_IslandRumble" (Variables|Transformation|GetRootComponent) "None" "0, 0, 0" "0, 0, 0" "KeepRelativeOffset" true))
      (bind _output_get_3 (Variables|Default|SetNS_IslandRumble _returnvalue_2))
      (Class|NiagaraDataInterfaceArrayFunctionLibrary|SetNiagaraArrayPosition _output_get_3 "Vertices" (.topvertices (Variables|Default|GetID)))
      (Niagara|SetNiagaraVariable(Float) _output_get_3 "IslandSizeRatio" (Variables|Default|GetIslandSize))
      (else
        (Class|AudioParameterControllerInterface|SetTriggerParameter (Variables|Default|GetAudioRumble) "RumbleStop")
        (Utilities|FlowControl|Sequence
          (:then_0
            (Utilities|IsValid (Variables|Default|GetCS_Rumble)
              (:Is%20Valid
                (CameraShake|StopAllCameraShakes (Variables|Default|GetCS_Rumble) false)
                (Components|DestroyComponent (Variables|Default|GetCS_Rumble)))))
          (:then_1
            (Utilities|IsValid (Variables|Default|GetNS_IslandRumble)
              (:Is%20Valid
                (Components|Activation|SetActive (Variables|Default|GetNS_IslandRumble) false false)))))))))

(fn Crystallize
  (if (>= (Class|PlayerIsland|GetEssence) (Variables|ConfigVariables|GetCrystallizeCost))
    (Class|PlayerIsland|SetEssence (- (Class|PlayerIsland|GetEssence) (/ (Variables|ConfigVariables|GetCrystallizeCost) 2)))
    (Class|PlayerIsland|SetIsCrystal true)))

(fn CheckResizeSpace
  (params (NewSize :type Integer))
  (bind _returnvalue (Transformation|GetActorLocation))
  (bind _outhits (Collision|MultiSphereTraceByChannel _returnvalue _returnvalue (Math|Conversions|ToFloat(Integer) (+ (* NewSize 100) 1200)) "TraceTypeQuery1" false (Actor|GetAttachedActors true true) "None" true "(R=1.000000,G=0.000000,B=0.000000,A=1.000000)" "(R=0.000000,G=1.000000,B=0.000000,A=1.000000)" 1.0))
  (for _array_element _outhits
    (if (Class|GameplayStatics|ObjectIsA (.HitActor (Collision|BreakHitResult _array_element)) "/Script/SkyCraft.Island")
      (return false)))
  (return true))