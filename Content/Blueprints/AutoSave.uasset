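; AutoSave is a component that periodically saves the world in shipping builds.
; On BeginPlay it caches its owner as BP_GMS, waits one tick interval, then enables its tick only if the build is shipping.
; Each tick calls SaveWorld on that owner, so the component's tick interval sets the autosave period.
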(event EventTick
  (params (DeltaSeconds :type Float%20%28single-precision%29))
  (Default|SaveWorld (Variables|Default|GetBP_GMS) false))

(event EventBeginPlay
  (bind _asbp_gms (Utilities|Casting|CastToBP_GMS (Components|GetOwner))
    (:then
      _)
    (:CastFailed
      _))
  (Variables|Default|SetBP_GMS _asbp_gms)
  (Utilities|FlowControl|Delay (Class|ActorComponent|GetComponentTickInterval))
  (if (Class|LowEntryExtendedStandardLibrary|ShippingBuild)
    (Components|Tick|SetComponentTickEnabled true)))