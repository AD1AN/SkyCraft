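; Actor component that tracks prolonged interact and edit sessions between its owner and a player's pawn.
; Enable functions store the pawn and controller and turn on tick, which switches off once neither session is active.
; Tick ends a session when its pawn is invalid or beyond a fixed range, sending client and server interrupt interface messages to the owner.
; A server event also multicasts clearing of the EditableWith list.
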(event Custom|Server_ClearEditableWith
  (CallFunction|MulticastClearEditablewith))

(event Custom|Multicast_ClearEditableWith
  (Utilities|Array|Clear (Variables|Interact2|GetEditableWith)))

(event EventTick
  (params (DeltaSeconds :type Float%20%28single-precision%29))
  (bind _self self)
  (bind _self_2 self)
  (bind _self_3 self)
  (bind _self_4 self)
  (bind _returnvalue (Components|GetOwner _self_2))
  (bind _returnvalue_2 (Components|GetOwner _self_4))
  (bind _returnvalue_3 (Components|GetOwner _self))
  (bind _returnvalue_4 (Components|GetOwner _self_3))
  (Utilities|FlowControl|Sequence
    (:then_0
      (if (Variables|Interact1|GetProlongedInteract)
        (Utilities|IsValid (Variables|Interact1|GetP_Interact_Pawn)
          (:Is%20Valid
            (if (> (Math|Vector|Distance(Vector) (Transformation|GetActorLocation (Components|GetOwner)) (Transformation|GetActorLocation (Variables|Interact1|GetP_Interact_Pawn))) 7e+02)
              (Class|BPIInteraction|INT1ClientInterrupt(Message) _returnvalue_3 (Variables|Interact1|GetP_Interact_Pawn) (Variables|Interact1|GetP_Interact_PC_Sky))
              (Class|BPIInteraction|INT1ServerInterrupt(Message) _returnvalue_3 (Variables|Interact1|GetP_Interact_Pawn) (Variables|Interact1|GetP_Interact_PC_Sky))
              (CallFunction|DisableProlongedInteract)))
          (:Is%20Not%20Valid
            (Class|BPIInteraction|INT1ClientInterrupt(Message) _returnvalue_2 0 (Variables|Interact1|GetP_Interact_PC_Sky))
            (Class|BPIInteraction|INT1ServerInterrupt(Message) _returnvalue_2 0 (Variables|Interact1|GetP_Interact_PC_Sky))
            (CallFunction|DisableProlongedInteract)))))
    (:then_1
      (if (Variables|Interact2|GetProlongedEdit)
        (Utilities|IsValid (Variables|Interact2|GetP_Edit_Pawn)
          (:Is%20Valid
            (if (> (Math|Vector|Distance(Vector) (Transformation|GetActorLocation (Components|GetOwner)) (Transformation|GetActorLocation (Variables|Interact2|GetP_Edit_Pawn))) 7e+02)
              (Class|BPIInteraction|INT2ClientInterrupt(Message) _returnvalue_4 (Variables|Interact2|GetP_Edit_Pawn) (Variables|Interact2|GetP_Edit_PC_Sky))
              (Class|BPIInteraction|INT2ServerInterrupt(Message) _returnvalue_4 (Variables|Interact2|GetP_Edit_Pawn) (Variables|Interact2|GetP_Edit_PC_Sky))
              (CallFunction|DisableProlongedEdit)))
          (:Is%20Not%20Valid
            (Class|BPIInteraction|INT2ClientInterrupt(Message) _returnvalue 0 (Variables|Interact2|GetP_Edit_PC_Sky))
            (Class|BPIInteraction|INT2ServerInterrupt(Message) _returnvalue 0 (Variables|Interact2|GetP_Edit_PC_Sky))
            (CallFunction|DisableProlongedEdit)))))
    (:then_2
      (if (and (not (Variables|Interact1|GetProlongedInteract)) (not (Variables|Interact2|GetProlongedEdit)))
        (Components|Tick|SetComponentTickEnabled false)))))

(fn EnableProlongedInteract
  (params (InteractedPawn :type Pawn%20Object%20Reference) (InteractedPC_Sky :type PC%20Sky%20Object%20Reference))
  (Variables|Interact1|SetP_Interact_Pawn InteractedPawn)
  (Variables|Interact1|SetP_Interact_PC_Sky InteractedPC_Sky)
  (Variables|Interact1|SetProlongedInteract true)
  (Components|Tick|SetComponentTickEnabled self true)
  (return))

(fn DisableProlongedInteract
  (Variables|Interact1|SetP_Interact_Pawn 0)
  (Variables|Interact1|SetP_Interact_PC_Sky 0)
  (Variables|Interact1|SetProlongedInteract false)
  (if (and (not (Variables|Interact1|GetProlongedInteract)) (not (Variables|Interact2|GetProlongedEdit)))
    (Components|Tick|SetComponentTickEnabled false)))

(fn EnableProlongedEdit
  (params (InteractedPawn :type Pawn%20Object%20Reference) (InteractedPC_Sky :type PC%20Sky%20Object%20Reference))
  (Variables|Interact2|SetP_Edit_Pawn InteractedPawn)
  (Variables|Interact2|SetP_Edit_PC_Sky InteractedPC_Sky)
  (Variables|Interact2|SetProlongedEdit true)
  (Components|Tick|SetComponentTickEnabled self true)
  (return))

(fn DisableProlongedEdit
  (Variables|Interact2|SetP_Edit_Pawn 0)
  (Variables|Interact2|SetP_Edit_PC_Sky 0)
  (Variables|Interact2|SetProlongedEdit false)
  (if (and (not (Variables|Interact1|GetProlongedInteract)) (not (Variables|Interact2|GetProlongedEdit)))
    (Components|Tick|SetComponentTickEnabled false)
    (return)))