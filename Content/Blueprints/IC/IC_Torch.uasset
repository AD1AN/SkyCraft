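; IC_Torch is the item component for a torch held in either hand.
; Starting it poses that arm through the anim Blueprint and attaches a spawned A_Torch to the hand socket, while server Tick applies burning durability; ending removes both.
; A multicast two-swing montage combo uses server-side box hits for damage and durability, stopping Tick on a hit.
; The attack trigger is disconnected, as left-click is still a todo stub.
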(event Custom|Server_Attack
  (CallFunction|MulticastAttack (Variables|Default|GetCombo)))

(event Custom|LMB%20PRESSED)

(event Custom|Multicast_StartYawInterp
  (bind _pf_normal (Variables|Default|GetPF_Normal))
  (Default|StartYawInterp (Variables|/Game/Blueprints/PF_Normal.PF_Normal_C|GetYawInterp _pf_normal) (.yaw (Variables|/Script/SkyCraft.PlayerNormal|GetLookRotation _pf_normal)) 9.0))

(event Custom|Server_StartYawInterp
  (CallFunction|MulticastStartYawInterp))

(event Custom|Multicast_Attack
  (params (Combo :type Integer))
  (Animation|Montage|PlayMontage (Variables|/Script/Engine.Character|GetMesh (Variables|Default|GetPF_Normal)) (select (> Combo 0) "/Game/Player/Animations/Male_SwordAttack2_Montage.Male_SwordAttack2_Montage" "/Game/Player/Animations/Male_SwordAttack1_Montage.Male_SwordAttack1_Montage")
    (:then
      (Networking|SwitchHasAuthority
        (:Authority
          (Variables|Default|SetCombo (select (> Combo 0) 0 1)))))
    (:OnNotifyBegin
      (Networking|SwitchHasAuthority
        (:Authority
          (Variables|Default|SetSwing true)
          (bind _hits (Default|BodyForwardMBox (Variables|Default|GetPF_Normal) 0.0 "TraceTypeQuery1"))
          (CallFunction|HitsApplyDamage _hits))))
    (:OnNotifyEnd
      (Variables|Default|SetCanLMB true)
      (Networking|SwitchHasAuthority
        (:Authority
          (if (Variables|Default|GetSwing)
            (Variables|Default|SetSwing false)))))))

(event EventTick
  (params (DeltaSeconds :type Float%20%28single-precision%29))
  (Class|DurabilityInterface|ApplyDurability(Message) (Variables|Default|GetPF_Normal) (Utilities|Struct|MakeApplyDurabilityIn "/Game/DataAssets/Durability/TorchBurning.TorchBurning" (Variables|Default|GetInventory) (Variables|Default|GetSlotIndex))))

(event EventEndItemComponent
  (bind _pf_normal (Variables|Default|GetPF_Normal))
  (bind _abp_normal (Variables|/Game/Blueprints/PF_Normal.PF_Normal_C|GetABP_Normal _pf_normal))
  (if (Variables|Default|GetMain)
    (Variables|/Game/Player/ABP_Normal.ABP_Normal_C|SetArm_R _abp_normal false)
    (else
      (Variables|/Game/Player/ABP_Normal.ABP_Normal_C|SetArm_L _abp_normal false)))
  (Actor|DestroyActor (Variables|Default|GetCreatedTorch)))

(event EventStartItemComponent
  (bind _pf_normal (Variables|Default|GetPF_Normal))
  (bind _abp_normal (Variables|/Game/Blueprints/PF_Normal.PF_Normal_C|GetABP_Normal _pf_normal))
  (if (Variables|Default|GetMain)
    (Variables|/Game/Player/ABP_Normal.ABP_Normal_C|SetAnimArm_R _abp_normal "/Game/Player/Animations/Male_ITAN_Torch.Male_ITAN_Torch")
    (Variables|/Game/Player/ABP_Normal.ABP_Normal_C|SetArm_R _abp_normal true)
    (Variables|/Game/Player/ABP_Normal.ABP_Normal_C|SetArm_R_Weight _abp_normal 0.9)
    (else
      (Variables|/Game/Player/ABP_Normal.ABP_Normal_C|SetAnimArm_L _abp_normal "/Game/Player/Animations/Male_ITAN_Torch.Male_ITAN_Torch")
      (Variables|/Game/Player/ABP_Normal.ABP_Normal_C|SetArm_L _abp_normal true)
      (Variables|/Game/Player/ABP_Normal.ABP_Normal_C|SetArm_L_Weight _abp_normal 0.9)))
  (bind _returnvalue (Game|SpawnActorfromClass "/Game/Blueprints/IC/A_Torch.A_Torch_C" (Math|Transform|MakeTransform "-8.000000,2.500000, 0" (select (Variables|Default|GetMain) "0, 0, 0" "0.000000,0.000000,180.000000") "1.000000,1.000000,1.000000") "AlwaysSpawn" "OverrideRootScale" 0 0))
  (bind _output_get (Variables|Default|SetCreatedTorch _returnvalue))
  (Transformation|AttachComponentToComponent _output_get (Variables|/Script/Engine.Character|GetMesh (Variables|Default|GetPF_Normal)) (select (Variables|Default|GetMain) "RightHand" "LeftHand") "KeepRelative" "KeepRelative" "KeepRelative" true)
  (Networking|SwitchHasAuthority
    (:Authority
      (Actor|Tick|SetActorTickEnabled true))))

(event EventLMB
  (params (Pressed :type Boolean))
  (if Pressed
    (CallFunction|LMBPRESSED)))

(fn OnRepCharNormal)

(fn HitsApplyDamage
  (params (Hits :type Array%20of%20Hit%20Result%20Structures))
  (for _array_element Hits
    (bind _returnvalue (Class|AdianFL|DoDamage (.HitActor (Collision|BreakHitResult _array_element)) (Utilities|Struct|MakeDamageInfo "/Game/DataAssets/DamageAction/WoodenTorch.WoodenTorch" (Variables|Default|GetPF_Normal) (.ImpactPoint (Collision|BreakHitResult _array_element)) 0.0)))
    (if _returnvalue
      (Class|DurabilityInterface|ApplyDurability(Message) (Variables|Default|GetPF_Normal) (Utilities|Struct|MakeApplyDurabilityIn "/Game/DataAssets/Durability/StandardDamage.StandardDamage" 0 0))
      (Variables|Default|SetSwing false)
      (Actor|Tick|SetActorTickEnabled false)
      (return))))

(fn ConstructionScript)