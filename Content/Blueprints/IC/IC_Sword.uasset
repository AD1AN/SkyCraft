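; Sword item component that gives the player a stamina-gated, two-step melee combo.
; On start it poses the right arm, loads the damage action and attaches a weapon mesh actor.
; LMB sends a server attack that multicasts yaw interpolation and montage, temporarily trusting client movement; holding chains attacks.
; Montage notify starts the trail and server-only Tick box traces, which stop after a damaging hit that also costs durability.
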(event Custom|Server_Attack
  (params (TargetLook :type Float%20%28double-precision%29))
  (CallFunction|MulticastStartYawInterp TargetLook)
  (Default|AuthConsumeStamina (Variables|Default|GetPF_Normal) 5.0)
  (CallFunction|MulticastAttack (Variables|Default|GetCombo))
  (bind _output_get (Variables|Default|SetCombo (+ (Variables|Default|GetCombo) 1)))
  (if (== _output_get 2)
    (Variables|Default|SetCombo 0)))

(event Custom|Multicast_StartYawInterp
  (params (TargetYaw :type Float%20%28double-precision%29))
  (Default|StartYawInterp (Variables|/Game/Blueprints/PF_Normal.PF_Normal_C|GetYawInterp (Variables|Default|GetPF_Normal)) TargetYaw 9.0))

(event Custom|Multicast_Attack
  (params (Combo :type Byte))
  (bind _pf_normal (Variables|Default|GetPF_Normal))
  (bind _basicweapon (Variables|Default|GetBasicWeapon))
  (bind _pf_normal_2 (Variables|Default|GetPF_Normal))
  (bind _pf_normal_3 (Variables|Default|GetPF_Normal))
  (bind _pf_normal_4 (Variables|Default|GetPF_Normal))
  (bind _ns_weapontrail (Variables|/Game/Blueprints/IC/BasicWeapon.BasicWeapon_C|GetNS_WeaponTrail _basicweapon))
  (bind _charactermovement (Variables|/Script/Engine.Character|GetCharacterMovement _pf_normal_3))
  (bind _charactermovement_2 (Variables|/Script/Engine.Character|GetCharacterMovement _pf_normal_2))
  (Variables|/Script/Engine.CharacterMovementComponent|SetbIgnoreClientMovementErrorChecksAndCorrection _charactermovement_2 true)
  (Variables|/Script/Engine.CharacterMovementComponent|SetbServerAcceptClientAuthoritativePosition _charactermovement_2 true)
  (Variables|Default|SetCanLMB false)
  (Variables|/Game/Player/ABP_Normal.ABP_Normal_C|SetArm_R (Variables|/Game/Blueprints/PF_Normal.PF_Normal_C|GetABP_Normal (Variables|Default|GetPF_Normal)) false)
  (Variables|/Game/Blueprints/PF_Normal.PF_Normal_C|SetAnimLookAt _pf_normal false)
  (|AdianPlayMontage (Variables|/Script/Engine.Character|GetMesh _pf_normal) (Utilities|Select :Index Combo :Option%200 "/Game/Player/Animations/Male_SwordAttack1_Montage.Male_SwordAttack1_Montage" :Option%201 "/Game/Player/Animations/Male_SwordAttack2_Montage.Male_SwordAttack2_Montage") 1.0 0.0 "None" true
    (:OnCompleted
      (Variables|Default|SetCombo 0))
    (:OnBlendOut
      (Components|Activation|SetActive _ns_weapontrail false false :!label _label)
      (Variables|/Game/Player/ABP_Normal.ABP_Normal_C|SetArm_R (Variables|/Game/Blueprints/PF_Normal.PF_Normal_C|GetABP_Normal _pf_normal_4) true)
      (Variables|/Game/Blueprints/PF_Normal.PF_Normal_C|SetAnimLookAt _pf_normal_4 true)
      (Variables|Default|SetCanLMB true)
      (Variables|/Script/Engine.CharacterMovementComponent|SetbIgnoreClientMovementErrorChecksAndCorrection _charactermovement false)
      (Variables|/Script/Engine.CharacterMovementComponent|SetbServerAcceptClientAuthoritativePosition _charactermovement false)
      (Utilities|FlowControl|Sequence
        (:then_0
          (Networking|SwitchHasAuthority
            (:Authority
              (Actor|Tick|SetActorTickEnabled false))))
        (:then_1
          (if (Class|PSS|IsLocalState (Variables|/Game/Blueprints/PF_Normal.PF_Normal_C|GetBP_PSS (Variables|Default|GetPF_Normal)))
            (if (Variables|Default|GetLMB_Pressed)
              (CallFunction|ServerAttack (.yaw (Variables|/Script/SkyCraft.PlayerNormal|GetLookRotation (Variables|Default|GetPF_Normal)))))))))
    (:OnInterrupted
      (goto _label))
    (:OnNotifyBegin
      (Components|Activation|SetActive _ns_weapontrail true false)
      (Networking|SwitchHasAuthority
        (:Authority
          (Actor|Tick|SetActorTickEnabled true))))))

(event EventTick
  (params (DeltaSeconds :type Float%20%28single-precision%29))
  (bind _hits (Default|BodyForwardMBox (Variables|Default|GetPF_Normal) 0.0 "TraceTypeQuery5"))
  (CallFunction|HitsApplyDamage _hits))

(event EventStartItemComponent
  (bind _pf_normal (Variables|Default|GetPF_Normal))
  (bind _abp_normal (Variables|/Game/Blueprints/PF_Normal.PF_Normal_C|GetABP_Normal _pf_normal))
  (Variables|/Game/Player/ABP_Normal.ABP_Normal_C|SetAnimArm_R _abp_normal "/Game/Player/Animations/Male_ITAN_Sword.Male_ITAN_Sword")
  (Variables|/Game/Player/ABP_Normal.ABP_Normal_C|SetArm_R _abp_normal true)
  (Variables|/Game/Player/ABP_Normal.ABP_Normal_C|SetArm_R_Weight _abp_normal 0.9)
  (bind _object (Utilities|AsyncLoadAsset (Utilities|Array|Get(acopy) (Utilities|Struct|BreakItemComponentParameters (Variables|/Script/SkyCraft.DA_Item|GetItemComponentParameters (Variables|Default|GetDA_Item)))))
    (:then
      (bind _returnvalue (Utilities|LoadAssetBlocking (Utilities|Array|Get(acopy) (Utilities|Struct|BreakItemComponentParameters (Variables|/Script/SkyCraft.DA_Item|GetItemComponentParameters (Variables|Default|GetDA_Item))) 1)))
      (bind _asda_damage_action (Utilities|Casting|CastToDA_DamageAction _returnvalue))
      (Variables|Default|SetDA_DamageAction _asda_damage_action))
    (:Completed
      (bind _asstatic_mesh (Utilities|Casting|CastToStaticMesh _object))
      (bind _returnvalue_2 (Game|SpawnActorfromClass "/Game/Blueprints/IC/BasicWeapon.BasicWeapon_C" (Math|Transform|MakeTransform "-7.000000,1.500000,0.000000" "0.000000,0.000000,-90.000000" "1.000000,1.000000,1.000000") "AlwaysSpawn" "MultiplyWithRoot" 0 _asstatic_mesh (Variables|/Script/Engine.Character|GetMesh (Variables|Default|GetPF_Normal)) true 0))
      (Variables|Default|SetBasicWeapon _returnvalue_2))))

(event EventEndItemComponent
  (Variables|/Game/Player/ABP_Normal.ABP_Normal_C|SetArm_R (Variables|/Game/Blueprints/PF_Normal.PF_Normal_C|GetABP_Normal (Variables|Default|GetPF_Normal)) false)
  (Variables|/Game/Blueprints/PF_Normal.PF_Normal_C|SetAnimLookAt (Variables|Default|GetPF_Normal) true) ; in future, change to list
  (Actor|DestroyActor (Variables|Default|GetBasicWeapon)))

(event EventLMB
  (params (Pressed :type Boolean))
  (if Pressed
    (if (Math|Boolean|ANDBoolean (Variables|Default|GetCanLMB) (not (AI|Components|NavMovement|IsFalling (Variables|/Script/Engine.Character|GetCharacterMovement (Variables|Default|GetPF_Normal)))) (> (Variables|/Script/SkyCraft.PlayerNormal|GetStamina (Variables|Default|GetPF_Normal)) 6.0))
      (Variables|Default|SetCanLMB false)
      (CallFunction|ServerAttack (.yaw (Variables|/Script/SkyCraft.PlayerNormal|GetLookRotation (Variables|Default|GetPF_Normal)))))))

(fn OnRepCharNormal)

(fn HitsApplyDamage
  (params (Hits :type Array%20of%20Hit%20Result%20Structures))
  (for _array_element Hits
    (bind _returnvalue (Class|AdianFL|DoDamage (.HitActor (Collision|BreakHitResult _array_element)) (Utilities|Struct|MakeDamageInfo (Variables|Default|GetDA_DamageAction) (Variables|Default|GetPF_Normal) (.ImpactPoint (Collision|BreakHitResult _array_element)) 0.0)))
    (if _returnvalue
      (Class|DurabilityInterface|ApplyDurability(Message) (Variables|Default|GetPF_Normal) (Utilities|Struct|MakeApplyDurabilityIn "/Game/DataAssets/Durability/StandardDamage.StandardDamage" (Variables|Default|GetInventory) (Variables|Default|GetSlotIndex)))
      (Actor|Tick|SetActorTickEnabled false))))

(fn ConstructionScript)