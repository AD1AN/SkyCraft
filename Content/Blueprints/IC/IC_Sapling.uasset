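; Item component for a sapling that the player holds in the right hand and plants on islands.
; The local player gets a tick-traced green/red preview, valid only on unobstructed procedural island terrain that is not too steep.
; LMB sends an island-local location and random yaw to the server, which multicasts planting FX, spawns a growing resource, then consumes the item.
; FX runs first because consuming the item destroys the component.
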(event Custom|Server_PlantSapling
  (params (Location :type Vector%20Net%20Quantize%20Structure) (Island :type Island%20Object%20Reference) (YawRotation :type Float%20%28single-precision%29))
  (bind _object (Utilities|AsyncLoadAsset (Utilities|Array|Get(acopy) (Utilities|Struct|BreakItemComponentParameters (Variables|/Script/SkyCraft.DA_Item|GetItemComponentParameters (Variables|Default|GetDA_Item))) 1))
    (:Completed
      (bind _asda_resource (Utilities|Casting|CastToDA_Resource _object))
      (CallFunction|MulticastPlantFX Island Location) ; should be first, otherwise it will\nnot happen due IC destroyed.
      (Class|GMS|SpawnResource (Variables|/Game/Blueprints/BP_GSS.BP_GSS_C|GetBP_GMS (Variables|Default|GetBP_GSS)) Island Location (Math|Rotator|MakeRotator 0.0 0.0 YawRotation) _asda_resource 0 true -1)
      (Class|InventoryComponent|ConsumeSingle (Variables|/Script/SkyCraft.PlayerNormal|GetInventoryComponent (Variables|Default|GetPF_Normal)) (Variables|Default|GetSlotIndex)))))

(event Custom|Multicast_PlantFX
  (params (Island :type Island%20Object%20Reference) (Location :type Vector%20Net%20Quantize%20Structure))
  (Audio|SpawnSoundAttached "/Game/Audio/SFX/Mattock_AddFoliage.Mattock_AddFoliage" (Variables|/Script/Engine.Actor|GetRootComponent Island) "None" Location "0, 0, 0" "KeepRelativeOffset" false 1.0 (Math|Random|RandomFloatinRange 0.9 1.1) 0.0 "/Game/Audio/NormalAttenuation.NormalAttenuation" 0)
  (Animation|Montage|PlayMontage (Variables|/Script/Engine.Character|GetMesh (Variables|Default|GetPF_Normal)) "/Game/Player/Animations/Male_Planting_Montage.Male_Planting_Montage"))

(event EventLMB
  (params (Pressed :type Boolean))
  (bind _island (Variables|Default|GetIsland))
  (bind _previewlocation (Variables|Default|GetPreviewLocation))
  (bind _returnvalue (Transformation|GetActorTransform _island))
  (bind _returnvalue_2 (Math|Transform|InverseTransformLocation _returnvalue _previewlocation))
  (if Pressed
    (if (Variables|Default|GetCanPlant)
      (CallFunction|ServerPlantSapling (Math|Vector|MakeVectorNetQuantize (.x _returnvalue_2) (.y _returnvalue_2) (.z _returnvalue_2)) _island (Variables|Default|GetPreviewRotation)))))

(event EventStartItemComponent
  (bind _object (Utilities|AsyncLoadAsset (Utilities|Array|Get(acopy) (Utilities|Struct|BreakItemComponentParameters (Variables|/Script/SkyCraft.DA_Item|GetItemComponentParameters (Variables|Default|GetDA_Item)))))
    (:Completed
      (bind _asstatic_mesh (Utilities|Casting|CastToStaticMesh _object))
      (Variables|Default|SetSaplingMesh _asstatic_mesh)
      (bind _returnvalue (Game|AddComponentbyClass (Variables|Default|GetPF_Normal) "/Script/Engine.StaticMeshComponent" true (Math|Transform|MakeTransform "-8.000000,2.500000,0.000000" "0, 0, 0" "1.000000,1.000000,1.000000")))
      (bind _output_get (Variables|Default|SetStaticMeshComponent _returnvalue))
      (Components|StaticMesh|SetStaticMesh _output_get _asstatic_mesh)
      (Class|AdianFL|ResolveStaticMeshCustomPrimitiveData (Variables|Default|GetStaticMeshComponent))
      (Transformation|AttachComponentToComponent (Variables|Default|GetStaticMeshComponent) (Variables|/Script/Engine.Character|GetMesh (Variables|Default|GetPF_Normal)) "RightHand" "KeepRelative" "KeepRelative" "KeepRelative" false)
      (if (CallFunction|IsLocallyControlled)
        (Actor|Tick|SetActorTickEnabled true)
        (bind _returnvalue_2 (Game|SpawnActorfromClass "/Game/Blueprints/IC/PreviewSapling.PreviewSapling_C" (Math|Transform|MakeTransform "0, 0, 0" "0, 0, 0" "1.000000,1.000000,1.000000") "AlwaysSpawn" "MultiplyWithRoot" 0 (Variables|Default|GetSaplingMesh) 0))
        (Variables|Default|SetPreviewSapling _returnvalue_2)
        (Variables|Default|SetPreviewRotation (Math|Random|RandomFloatinRange 0.0 3.6e+02))))))

(event EventTick
  (params (DeltaSeconds :type Float%20%28single-precision%29))
  (bind _pf_normal (Variables|Default|GetPF_Normal))
  (bind (_start _end) (Default|LineSizeCamera _pf_normal 1e+02))
  (Utilities|IsValid (Variables|Default|GetPreviewSapling)
    (:Is%20Valid
      (bind (_outhit _returnvalue) (Collision|LineTraceByChannel _start _end "TraceTypeQuery4" false 0 "None"))
      (bind _canplant1 (CallFunction|SetCanPlant _returnvalue))
      (bind _output_get (Variables|Default|SetPreviewLocation (select _canplant1 (.Location (Collision|BreakHitResult _outhit)) (.TraceEnd (Collision|BreakHitResult _outhit)))))
      (Transformation|SetActorLocationAndRotation (Variables|Default|GetPreviewSapling) _output_get (Math|Rotator|MakeRotator 0.0 0.0 (Variables|Default|GetPreviewRotation)) false true)
      (bind _asisland (Utilities|Casting|CastToIsland (.HitActor (Collision|BreakHitResult _outhit)))
        (:then
          (Variables|Default|SetIsland _asisland)
          (Class|KismetSystemLibrary|IsObjectOfSoftClass (.HitComponent (Collision|BreakHitResult _outhit)) "/Script/ProceduralMeshComponent.ProceduralMeshComponent"
            (:True
              (bind _returnvalue_2 (Collision|MultiSphereTraceByChannel (Variables|Default|GetPreviewLocation) (Variables|Default|GetPreviewLocation) 1e+02 "TraceTypeQuery4" false (Utilities|Array|MakeArray (Variables|Default|GetIsland)) "None"))
              (CallFunction|SetCanPlant (and (not _returnvalue_2) (<= (Class|KismetMathLibrary|DegAcos (Math|Vector|DotProduct (.ImpactNormal (Collision|BreakHitResult _outhit)) "0.000000,0.000000,1.000000")) 45.0))))
            (:False
              (CallFunction|SetCanPlant false :!label _label))))
        (:CastFailed
          (goto _label))))))

(event EventEndItemComponent
  (Class|AdianFL|ForceDestroyComponent (Variables|Default|GetStaticMeshComponent))
  (if (CallFunction|IsLocallyControlled)
    (Actor|DestroyActor (Variables|Default|GetPreviewSapling))))

(fn ConstructionScript)

(fn SetCanPlant
  (params (CanPlant :type Boolean))
  (bind _output_get (Variables|Default|SetCanPlant CanPlant))
  (Rendering|Material|SetVectorParameterValueonMaterials (Variables|/Game/Blueprints/IC/PreviewSapling.PreviewSapling_C|GetStaticMeshComponent (Variables|Default|GetPreviewSapling)) "BuildingPreviewColor" (select _output_get "0.000000,1.000000,0.000000" "1.000000,0.000000,0.000000"))
  (return (Variables|Default|GetCanPlant)))