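; Held-item component for a hand stone that the character swings as a melee weapon.
; Equipping attaches a collisionless stone mesh to the right hand and enables arm pose overrides, both undone on unequip.
; Held LMB, polled on the local client's Tick, repeats grounded swings through a server-to-multicast montage.
; The montage notify runs an authority-only box trace aimed by look rotation and crouch for Strike damage, plus a local camera shake.
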(event Custom|Server_Swing
  (CallFunction|MulticastSwing))

(event Custom|Multicast_Swing
  (bind _pf_normal (Variables|Default|GetPF_Normal))
  (bind _pf_normal_2 (Variables|Default|GetPF_Normal))
  (bind _abp_normal (Variables|/Game/Blueprints/PF_Normal.PF_Normal_C|GetABP_Normal _pf_normal))
  (bind _abp_normal_2 (Variables|/Game/Blueprints/PF_Normal.PF_Normal_C|GetABP_Normal _pf_normal_2))
  (Variables|/Game/Player/ABP_Normal.ABP_Normal_C|SetArm_R _abp_normal_2 false)
  (Variables|/Game/Player/ABP_Normal.ABP_Normal_C|SetArm_L _abp_normal_2 false)
  (|AdianPlayMontage (Variables|/Script/Engine.Character|GetMesh (Variables|Default|GetPF_Normal)) "/Game/Player/Animations/Male_HandStoneAttack_Montage.Male_HandStoneAttack_Montage" 1.0 0.0 "None" true
    (:OnBlendOut
      (Variables|/Game/Player/ABP_Normal.ABP_Normal_C|SetArm_R _abp_normal true :!label _label)
      (Variables|/Game/Player/ABP_Normal.ABP_Normal_C|SetArm_L _abp_normal true)
      (Variables|Default|SetCanLMB true))
    (:OnInterrupted
      (goto _label))
    (:OnNotifyBegin
      (Utilities|FlowControl|Sequence
        (:then_0
          (Networking|SwitchHasAuthority
            (:Authority
              (bind (_ishit _hit) (CallFunction|HitBoxTrace))
              (if _ishit
                (Class|AdianFL|DoDamage (.HitActor (Collision|BreakHitResult _hit)) (Utilities|Struct|MakeApplyDamageIn (Math|Random|RandomIntegerinRange 2222 2222) "Strike" "/Game/DataAssets/Item/I_Stone.I_Stone" (Variables|Default|GetPF_Normal) (.ImpactPoint (Collision|BreakHitResult _hit)) true))))))
        (:then_1
          (if (CallFunction|IsLocallyControlled)
            (CameraShakes|StartCameraShake (Variables|/Script/Engine.PlayerController|GetPlayerCameraManager (Variables|/Game/Blueprints/BP_PSS.BP_PSS_C|GetBP_PCS (Variables|Default|GetBP_PSS))) "/Game/Blueprints/CameraShake/CS_LittleImpact.CS_LittleImpact_C" 1.0 "CameraLocal" "0, 0, 0")))))))

(event EventEndItemComponent
  (bind _pf_normal (Variables|Default|GetPF_Normal))
  (bind _abp_normal (Variables|/Game/Blueprints/PF_Normal.PF_Normal_C|GetABP_Normal _pf_normal))
  (Variables|/Game/Player/ABP_Normal.ABP_Normal_C|SetArm_R _abp_normal false)
  (Variables|/Game/Player/ABP_Normal.ABP_Normal_C|SetArm_L _abp_normal false)
  (Class|AdianFL|ForceDestroyComponent (Variables|Default|GetStaticMesh)))

(event EventTick
  (params (DeltaSeconds :type Float%20%28single-precision%29))
  (if (Math|Boolean|ANDBoolean (Variables|Default|GetpressedLMB) (Variables|Default|GetCanLMB) (not (AI|Components|NavMovement|IsFalling (Variables|/Script/Engine.Character|GetCharacterMovement (Variables|Default|GetPF_Normal)))))
    (Variables|Default|SetCanLMB false)
    (CallFunction|ServerSwing)))

(event EventLMB
  (params (Pressed :type Boolean))
  (Variables|Default|SetpressedLMB Pressed))

(event EventStartItemComponent
  (bind _pf_normal (Variables|Default|GetPF_Normal))
  (bind _abp_normal (Variables|/Game/Blueprints/PF_Normal.PF_Normal_C|GetABP_Normal _pf_normal))
  (Variables|/Game/Player/ABP_Normal.ABP_Normal_C|SetAnimArm_R _abp_normal "/Game/Player/Animations/Male_ITAN_HandStone.Male_ITAN_HandStone")
  (Variables|/Game/Player/ABP_Normal.ABP_Normal_C|SetAnimArm_L _abp_normal "/Game/Player/Animations/Male_ITAN_HandStone.Male_ITAN_HandStone")
  (Variables|/Game/Player/ABP_Normal.ABP_Normal_C|SetArm_R _abp_normal true)
  (Variables|/Game/Player/ABP_Normal.ABP_Normal_C|SetArm_L _abp_normal true)
  (Variables|/Game/Player/ABP_Normal.ABP_Normal_C|SetArm_R_Weight _abp_normal 1.0)
  (Utilities|FlowControl|Sequence
    (:then_0
      (bind _returnvalue (Game|AddComponentbyClass (Variables|Default|GetPF_Normal) "/Script/Engine.StaticMeshComponent" true (Math|Transform|MakeTransform "-7.000000,13.000000,0.000000" "90.000000,0.000000,0.000000" "1.000000,1.000000,1.000000")))
      (bind _output_get (Variables|Default|SetStaticMesh _returnvalue))
      (Components|StaticMesh|SetStaticMesh _output_get "/Game/s2u/Stone.Stone")
      (Collision|SetCollisionEnabled _output_get "NoCollision")
      (Class|AdianFL|ResolveStaticMeshCustomPrimitiveData (Variables|Default|GetStaticMesh))
      (Transformation|AttachComponentToComponent (Variables|Default|GetStaticMesh) (Variables|/Script/Engine.Character|GetMesh (Variables|Default|GetPF_Normal)) "RightHand" "KeepRelative" "KeepRelative" "KeepRelative" false))
    (:then_1
      (if (CallFunction|IsLocallyControlled)
        (Actor|Tick|SetActorTickEnabled true)))))

(fn SetInputs
  (params (canMove :type Boolean) (canQSPressing :type Boolean) (canSpirit :type Boolean) (canInteract :type Boolean))
  (bind _pf_normal (Variables|Default|GetPF_Normal))
  (Variables|/Game/Blueprints/PF_Normal.PF_Normal_C|SetcanMove _pf_normal canMove)
  (Variables|/Game/Blueprints/PF_Normal.PF_Normal_C|SetcanQSPressing _pf_normal canQSPressing)
  (Variables|/Game/Blueprints/PF_Normal.PF_Normal_C|SetcanSpirit _pf_normal canSpirit)
  (Variables|/Game/Blueprints/PF_Normal.PF_Normal_C|SetcanInteract _pf_normal canInteract))

(fn EqualResource
  (params (Resource1 :type DA%20Resource%20Object%20Reference) (Resource2 :type DA%20Resource%20Object%20Reference) (NewParam :type Map%20of%20DA%20Resource%20Object%20References%20to%20Integers))
  (return (== Resource1 Resource2)))

(fn HitBoxTrace
  (bind _pf_normal (Variables|Default|GetPF_Normal))
  (bind _pf_normal_2 (Variables|Default|GetPF_Normal))
  (bind _pf_normal_3 (Variables|Default|GetPF_Normal))
  (bind _pf_normal_4 (Variables|Default|GetPF_Normal))
  (bind _returnvalue (Transformation|GetActorLocation _pf_normal_2))
  (bind _returnvalue_2 (Transformation|GetActorRotation _pf_normal_3))
  (bind _biscrouched (Variables|/Script/Engine.Character|GetbIsCrouched _pf_normal))
  (bind _lookrotation (Variables|/Game/Blueprints/PF_Normal.PF_Normal_C|GetLookRotation _pf_normal_3))
  (bind _biscrouched_2 (Variables|/Script/Engine.Character|GetbIsCrouched _pf_normal_4))
  (bind _returnvalue_3 (* (.yaw _lookrotation) -0.05))
  (bind _returnvalue_4 (select _biscrouched_2 1e+01 4e+01))
  (bind _returnvalue_5 (select _biscrouched 0.75 0.35))
  (bind _returnvalue_6 (+ _returnvalue (Math|Vector|MakeVector 0.0 0.0 _returnvalue_4)))
  (bind _returnvalue_7 (* (.pitch _lookrotation) _returnvalue_5))
  (bind _returnvalue_8 (+ (.yaw _returnvalue_2) _returnvalue_3))
  (bind _returnvalue_9 (Math|Rotator|MakeRotator (.roll _returnvalue_2) _returnvalue_7 _returnvalue_8))
  (bind _returnvalue_10 (Math|Vector|GetForwardVector _returnvalue_9))
  (bind (_outhit _returnvalue_11) (Collision|BoxTraceByChannel (+ _returnvalue_6 (* _returnvalue_10 2e+01)) (+ _returnvalue_6 (* _returnvalue_10 1e+02)) "1.000000,23.000000,23.000000" _returnvalue_9 "TraceTypeQuery1" false (Utilities|Array|MakeArray (Variables|Default|GetPF_Normal)) "None" false))
  (return _returnvalue_11 _outhit))

(fn ConstructionScript)