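; Item component for a wieldable axe that chops trees and swings as a networked melee weapon.
; On start it loads and attaches the weapon mesh; LMB chops a tree found by a forward box trace, otherwise spends stamina on an attack.
; Server RPCs multicast alternating combo montages, whose notifies let the authority deal damage and durability wear, directly for chops or via per-tick traces for attacks.
; Attacks temporarily accept client-authoritative movement.
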(event Custom|Server_Chop
  (params (TreeActor :type Actor%20Object%20Reference) (HitLocalLocation :type Vector))
  (CallFunction|MulticastChop TreeActor HitLocalLocation (Variables|Default|GetComboChop)))

(event Custom|Client_StopSwinging
  (CallFunction|SetInputs true true true true)
  (Variables|Default|SetCanLMB true))

(event Custom|Multicast_Chop
  (params (TreeActor :type Actor%20Object%20Reference) (HitLocalLocation :type Vector) (ComboChop :type Byte))
  (bind _pf_normal (Variables|Default|GetPF_Normal))
  (bind _pf_normal_2 (Variables|Default|GetPF_Normal))
  (Utilities|IsValid TreeActor
    (:Is%20Valid
      (Animation|Montage|PlayMontage (Variables|/Script/Engine.Character|GetMesh (Variables|Default|GetPF_Normal)) (Utilities|Select :Index ComboChop :Option%200 "/Game/Player/Animations/Male_Axe_Chop_First_Montage.Male_Axe_Chop_First_Montage" :Option%201 "/Game/Player/Animations/Male_Axe_Chop_Second_Montage.Male_Axe_Chop_Second_Montage")
        (:then
          (Variables|/Game/Player/ABP_Normal.ABP_Normal_C|SetHand_R (Variables|/Game/Blueprints/PF_Normal.PF_Normal_C|GetABP_Normal _pf_normal) false)
          (Variables|/Game/Blueprints/PF_Normal.PF_Normal_C|SetAnimLookAt _pf_normal false)
          (Utilities|IsValid TreeActor
            (:Is%20Valid
              (Default|StartYawInterp (Variables|/Game/Blueprints/PF_Normal.PF_Normal_C|GetYawInterp (Variables|Default|GetPF_Normal)) (.yaw (Math|Rotator|FindLookatRotation (Transformation|GetActorLocation (Variables|Default|GetPF_Normal)) (Transformation|GetActorLocation TreeActor))) 8.0)
              (if (== (Variables|Default|GetComboChop) 0)
                (Variables|Default|SetComboChop 1)))))
        (:OnCompleted
          (Variables|Default|SetComboChop 0))
        (:OnBlendOut
          (Variables|/Game/Player/ABP_Normal.ABP_Normal_C|SetHand_R (Variables|/Game/Blueprints/PF_Normal.PF_Normal_C|GetABP_Normal _pf_normal_2) true)
          (Variables|/Game/Blueprints/PF_Normal.PF_Normal_C|SetAnimLookAt _pf_normal_2 true))
        (:OnNotifyBegin
          (Utilities|FlowControl|Sequence
            (:then_0
              (Variables|Default|SetCanLMB true)
              (Networking|SwitchHasAuthority
                (:Authority
                  (CallFunction|DoDamage TreeActor (+ (Transformation|GetActorLocation TreeActor) HitLocalLocation))
                  (Class|DurabilityInterface|ApplyDurability(Message) (Variables|Default|GetPF_Normal) (Utilities|Struct|MakeApplyDurabilityIn "/Game/DataAssets/Durability/StandardDamage.StandardDamage" (Variables|Default|GetInventory) (Variables|Default|GetSlotIndex)))
                  (CallFunction|ClientStopSwinging))))
            (:then_1
              (if (CallFunction|IsLocallyControlled)
                (CameraShakes|StartCameraShake (Variables|/Script/Engine.PlayerController|GetPlayerCameraManager (Variables|/Game/Blueprints/BP_PSS.BP_PSS_C|GetBP_PCS (Variables|Default|GetBP_PSS))) "/Game/Blueprints/CameraShake/CS_LittleImpact.CS_LittleImpact_C" 1.0 "World" "0, 0, 0")
                (CallFunction|SetInputs true true true true)))))))))

(event Custom|Multicast_StartYawInterp
  (params (TargetYaw :type Float%20%28double-precision%29))
  (Default|StartYawInterp (Variables|/Game/Blueprints/PF_Normal.PF_Normal_C|GetYawInterp (Variables|Default|GetPF_Normal)) TargetYaw 9.0))

(event Custom|Multicast_Attack
  (params (ComboAttack :type Byte))
  (bind _pf_normal (Variables|Default|GetPF_Normal))
  (bind _pf_normal_2 (Variables|Default|GetPF_Normal))
  (bind _basicweapon (Variables|Default|GetBasicWeapon))
  (bind _pf_normal_3 (Variables|Default|GetPF_Normal))
  (bind _pf_normal_4 (Variables|Default|GetPF_Normal))
  (bind _charactermovement (Variables|/Script/Engine.Character|GetCharacterMovement _pf_normal_2))
  (bind _ns_weapontrail (Variables|/Game/Blueprints/IC/BasicWeapon.BasicWeapon_C|GetNS_WeaponTrail _basicweapon))
  (bind _charactermovement_2 (Variables|/Script/Engine.Character|GetCharacterMovement _pf_normal_4))
  (Variables|/Script/Engine.CharacterMovementComponent|SetbIgnoreClientMovementErrorChecksAndCorrection _charactermovement_2 true)
  (Variables|/Script/Engine.CharacterMovementComponent|SetbServerAcceptClientAuthoritativePosition _charactermovement_2 true)
  (Audio|SpawnSoundAttached "/Game/Audio/SFX/whoosh1.whoosh1" (Variables|/Script/Engine.Actor|GetRootComponent (Variables|Default|GetBasicWeapon)) "None" "0, 0, 0" "0, 0, 0" "KeepRelativeOffset" false 1.0 (Math|Random|RandomFloatinRange 0.9 1.1) 0.0 "/Game/Audio/NormalAttenuation.NormalAttenuation" 0)
  (Variables|Default|SetCanLMB false)
  (Variables|/Game/Player/ABP_Normal.ABP_Normal_C|SetHand_R (Variables|/Game/Blueprints/PF_Normal.PF_Normal_C|GetABP_Normal _pf_normal_3) false)
  (Variables|/Game/Blueprints/PF_Normal.PF_Normal_C|SetAnimLookAt _pf_normal_3 false)
  (|AdianPlayMontage (Variables|/Script/Engine.Character|GetMesh (Variables|Default|GetPF_Normal)) (Utilities|Select :Index ComboAttack :Option%200 "/Game/Player/Animations/Male_SwordAttack1_Montage.Male_SwordAttack1_Montage" :Option%201 "/Game/Player/Animations/Male_SwordAttack2_Montage.Male_SwordAttack2_Montage") 1.0 0.0 "None" true
    (:then
      (if (== (Variables|Default|GetComboAttack) 0)
        (Variables|Default|SetComboAttack 1)
        (else
          (Variables|Default|SetComboAttack 0))))
    (:OnCompleted
      (Variables|Default|SetComboAttack 0))
    (:OnBlendOut
      (Components|Activation|SetActive _ns_weapontrail false false :!label _label)
      (Variables|/Game/Player/ABP_Normal.ABP_Normal_C|SetHand_R (Variables|/Game/Blueprints/PF_Normal.PF_Normal_C|GetABP_Normal _pf_normal) true)
      (Variables|/Game/Blueprints/PF_Normal.PF_Normal_C|SetAnimLookAt _pf_normal true)
      (Variables|/Script/Engine.CharacterMovementComponent|SetbIgnoreClientMovementErrorChecksAndCorrection _charactermovement false)
      (Variables|/Script/Engine.CharacterMovementComponent|SetbServerAcceptClientAuthoritativePosition _charactermovement false)
      (Variables|Default|SetCanLMB true)
      (CallFunction|SetInputs true true true true)
      (Networking|SwitchHasAuthority
        (:Authority
          (Variables|Default|SetAttackSwing false))))
    (:OnInterrupted
      (goto _label))
    (:OnNotifyBegin
      (Components|Activation|SetActive _ns_weapontrail true false)
      (Networking|SwitchHasAuthority
        (:Authority
          (Variables|Default|SetAttackSwing true))))))

(event Custom|Server_Attack
  (params (TargetYaw :type Float%20%28double-precision%29))
  (CallFunction|MulticastStartYawInterp TargetYaw)
  (Default|AuthConsumeStamina (Variables|Default|GetPF_Normal) 3.0)
  (CallFunction|MulticastAttack (Variables|Default|GetComboAttack)))

(event EventTick
  (params (DeltaSeconds :type Float%20%28single-precision%29))
  (CallFunction|ResourceChopTick)
  (if (Variables|Default|GetAttackSwing)
    (bind _hits (Default|BodyForwardMBox (Variables|Default|GetPF_Normal) 0.0 "TraceTypeQuery5"))
    (if (Utilities|Array|IsEmpty _hits)
      (bind _hits_2 (Default|BodyForwardMBox (Variables|Default|GetPF_Normal) 0.0 "TraceTypeQuery4"))
      (CallFunction|HitsApplyDamage _hits_2)
      (else
        (CallFunction|HitsApplyDamage _hits)))))

(event EventLMB
  (params (Pressed :type Boolean))
  (bind _output_get (Variables|Default|SetpressedLMB Pressed))
  (if (Math|Boolean|ANDBoolean _output_get (not (AI|Components|NavMovement|IsFalling (Variables|/Script/Engine.Character|GetCharacterMovement (Variables|Default|GetPF_Normal)))) (> (Variables|/Script/SkyCraft.PlayerNormal|GetStamina (Variables|Default|GetPF_Normal)) 5.0))
    (bind _resourcefound (CallFunction|ResourceChopTick))
    (if (and (not _resourcefound) (Variables|Default|GetCanLMB))
      (Variables|Default|SetpressedLMB false)
      (CallFunction|ServerAttack (.yaw (Variables|/Script/SkyCraft.PlayerNormal|GetLookRotation (Variables|Default|GetPF_Normal))))
      (Variables|Default|SetCanLMB false)
      (CallFunction|SetInputs false false false false))))

(event EventStartItemComponent
  (bind _pf_normal (Variables|Default|GetPF_Normal))
  (bind _abp_normal (Variables|/Game/Blueprints/PF_Normal.PF_Normal_C|GetABP_Normal _pf_normal))
  (Variables|/Game/Player/ABP_Normal.ABP_Normal_C|SetAnimArm_R _abp_normal "/Game/Player/Animations/Male_ITAN_StoneAxe.Male_ITAN_StoneAxe")
  (Variables|/Game/Player/ABP_Normal.ABP_Normal_C|SetHand_R _abp_normal true)
  (Utilities|FlowControl|Sequence
    (:then_0
      (bind _object (Utilities|AsyncLoadAsset (Utilities|Array|Get(acopy) (Utilities|Struct|BreakItemComponentParameters (Variables|/Script/SkyCraft.DA_Item|GetItemComponentParameters (Variables|Default|GetDA_Item)))))
        (:then
          (bind _returnvalue (Utilities|LoadAssetBlocking (Utilities|Array|Get(acopy) (Utilities|Struct|BreakItemComponentParameters (Variables|/Script/SkyCraft.DA_Item|GetItemComponentParameters (Variables|Default|GetDA_Item))) 1)))
          (bind _asda_damage_action (Utilities|Casting|CastToDA_DamageAction _returnvalue))
          (Variables|Default|SetDA_DamageAction _asda_damage_action))
        (:Completed
          (bind _asstatic_mesh (Utilities|Casting|CastToStaticMesh _object))
          (bind _returnvalue_2 (Game|SpawnActorfromClass "/Game/Blueprints/IC/BasicWeapon.BasicWeapon_C" (Math|Transform|MakeTransform "-7.000000,1.500000,0.000000" "0.000000,0.000000,-90.000000" "1.000000,1.000000,1.000000") "AlwaysSpawn" "MultiplyWithRoot" 0 _asstatic_mesh (Variables|/Script/Engine.Character|GetMesh (Variables|Default|GetPF_Normal)) true 0))
          (Variables|Default|SetBasicWeapon _returnvalue_2))))
    (:then_1
      (if (or (CallFunction|IsLocallyControlled) (Networking|IsServer))
        (Actor|Tick|SetActorTickEnabled true)))))

(event EventEndItemComponent
  (Actor|DestroyActor (Variables|Default|GetBasicWeapon))
  (Variables|/Game/Player/ABP_Normal.ABP_Normal_C|SetHand_R (Variables|/Game/Blueprints/PF_Normal.PF_Normal_C|GetABP_Normal (Variables|Default|GetPF_Normal)) false)
  (Variables|/Game/Blueprints/PF_Normal.PF_Normal_C|SetAnimLookAt (Variables|Default|GetPF_Normal) true)
  (if (CallFunction|IsLocallyControlled)
    (CallFunction|SetInputs true true true true)))

(fn SetInputs
  (params (canMove :type Boolean) (canQSPressing :type Boolean) (canSpirit :type Boolean) (canInteract :type Boolean))
  (bind _pf_normal (Variables|Default|GetPF_Normal))
  (Variables|/Game/Blueprints/PF_Normal.PF_Normal_C|SetcanMove _pf_normal canMove)
  (Variables|/Game/Blueprints/PF_Normal.PF_Normal_C|SetcanQSPressing _pf_normal canQSPressing)
  (Variables|/Game/Blueprints/PF_Normal.PF_Normal_C|SetcanSpirit _pf_normal canSpirit)
  (Variables|/Game/Blueprints/PF_Normal.PF_Normal_C|SetcanInteract _pf_normal canInteract))

(fn ResourceChopTick
  (if (Math|Boolean|ANDBoolean (Variables|Default|GetpressedLMB) (Variables|Default|GetCanLMB) (not (AI|Components|NavMovement|IsFalling (Variables|/Script/Engine.Character|GetCharacterMovement (Variables|Default|GetPF_Normal)))))
    (bind _hits (Default|BodyForwardMBox (Variables|Default|GetPF_Normal) -5e+01 "TraceTypeQuery1"))
    (bind _resourcefound (CallFunction|CheckResourcesAhead _hits))
    (return _resourcefound)))

(fn CheckResourcesAhead
  (params (Hits :type Array%20of%20Hit%20Result%20Structures))
  (for _array_element Hits
    (if (.Contains (CallFunction|ArrayContainsSkyTag (CallFunction|GetSkyTags (.HitActor (Collision|BreakHitResult _array_element))) (Utilities|Array|MakeArray "/Game/DataAssets/SkyTag/ST_Tree.ST_Tree")))
      (CallFunction|ServerChop (.HitActor (Collision|BreakHitResult _array_element)) (Class|AdianFL|ToLocalSpace (.ImpactPoint (Collision|BreakHitResult _array_element)) (.HitActor (Collision|BreakHitResult _array_element))))
      (Variables|Default|SetCanLMB false)
      (CallFunction|SetInputs false false false false)
      (return true))))

(fn ConstructionScript)

(fn HitsApplyDamage
  (params (Hits :type Array%20of%20Hit%20Result%20Structures))
  (for _array_element Hits
    (CallFunction|DoDamage (.HitActor (Collision|BreakHitResult _array_element)) (.ImpactPoint (Collision|BreakHitResult _array_element)))
    (Class|DurabilityInterface|ApplyDurability(Message) (Variables|Default|GetPF_Normal) (Utilities|Struct|MakeApplyDurabilityIn "/Game/DataAssets/Durability/StandardDamage.StandardDamage" (Variables|Default|GetInventory) (Variables|Default|GetSlotIndex)))
    (Variables|Default|SetAttackSwing false)
    (return)))

(fn DoDamage
  (params (DamageActor :type Actor%20Object%20Reference) (DamageLocation :type Vector))
  (Class|AdianFL|DoDamage DamageActor (Utilities|Struct|MakeDamageInfo (Variables|Default|GetDA_DamageAction) (Variables|Default|GetPF_Normal) DamageLocation 0.0)))