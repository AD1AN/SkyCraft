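; BP_IC is a Blueprint, bound to a normal player, that caches game and player state references and reports whether it is locally controlled.
; BeginPlay casts the game state to BP_GSS and PlayerNormal to PF_Normal, stopping if either cast fails.
; OnPostBeginPlay copies BPPSS from PFNormal before calling the parent implementation.
; IsLocallyControlled returns whether that BPPSS is the local player state.
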(event EventOnPostBeginPlay
  (Variables|Default|SetBP_PSS (Variables|/Game/Blueprints/PF_Normal.PF_Normal_C|GetBP_PSS (Variables|Default|GetPF_Normal)))
  (|CallParentFunction))

(event EventBeginPlay
  (bind _asbp_gss (Utilities|Casting|CastToBP_GSS (Game|GetGameState)))
  (Variables|Default|SetBP_GSS _asbp_gss)
  (bind _aspf_normal (Utilities|Casting|CastToPF_Normal (Variables|Default|GetPlayerNormal)))
  (Variables|Default|SetPF_Normal _aspf_normal))

(fn IsLocallyControlled
  (return (Default|IsLocalPlayerState (Variables|Default|GetBP_PSS))))

(fn ConstructionScript)