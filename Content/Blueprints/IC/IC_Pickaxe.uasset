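; Item component for a held pickaxe that lets the player swing to deal damage and wear down the tool.
; On start it sets arm poses, loads the mesh and damage action from the item data, and attaches the mesh to the right hand.
; Local Tick turns held LMB into server-to-multicast montage swings that lock movement.
; On the montage notify, the authority box-traces downward ahead of the player, applying damage and, on success, durability loss.
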(event Custom|Multicast_Swing
  (bind _pf_normal (Variables|Default|GetPF_Normal))
  (bind _pf_normal_2 (Variables|Default|GetPF_Normal))
  (bind _pf_normal_3 (Variables|Default|GetPF_Normal))
  (bind _pf_normal_4 (Variables|Default|GetPF_Normal))
  (bind _pf_normal_5 (Variables|Default|GetPF_Normal))
  (bind _returnvalue (Transformation|GetActorLocation _pf_normal_2))
  (bind _returnvalue_2 (Transformation|GetActorForwardVector _pf_normal_2))
  (bind _abp_normal (Variables|/Game/Blueprints/PF_Normal.PF_Normal_C|GetABP_Normal _pf_normal_4))
  (bind _abp_normal_2 (Variables|/Game/Blueprints/PF_Normal.PF_Normal_C|GetABP_Normal _pf_normal_3))
  (bind _returnvalue_3 (* _returnvalue_2 1e+02))
  (bind _returnvalue_4 (+ _returnvalue "0.000000,0.000000,100.000000"))
  (bind _returnvalue_5 (+ _returnvalue_4 _returnvalue_3))
  (Variables|/Game/Player/ABP_Normal.ABP_Normal_C|SetArm_R _abp_normal false)
  (Variables|/Game/Player/ABP_Normal.ABP_Normal_C|SetArm_L _abp_normal false)
  (Variables|/Game/Blueprints/PF_Normal.PF_Normal_C|SetcanMove _pf_normal_5 false)
  (Variables|/Game/Blueprints/PF_Normal.PF_Normal_C|SetcanQSPressing _pf_normal_5 false)
  (Variables|/Game/Blueprints/PF_Normal.PF_Normal_C|SetAnimLookAt (Variables|Default|GetPF_Normal) false)
  (Variables|Default|SetCanLMB false)
  (|AdianPlayMontage (Variables|/Script/Engine.Character|GetMesh (Variables|Default|GetPF_Normal)) "/Game/Player/Animations/Male_Pickaxe_Mine_Montage.Male_Pickaxe_Mine_Montage" 1.0 0.0 "None" true
    (:OnBlendOut
      (Variables|/Game/Player/ABP_Normal.ABP_Normal_C|SetArm_R _abp_normal_2 true :!label _label)
      (Variables|/Game/Player/ABP_Normal.ABP_Normal_C|SetArm_L _abp_normal_2 true)
      (Variables|/Game/Blueprints/PF_Normal.PF_Normal_C|SetcanMove _pf_normal true)
      (Variables|/Game/Blueprints/PF_Normal.PF_Normal_C|SetcanQSPressing _pf_normal true)
      (Variables|/Game/Blueprints/PF_Normal.PF_Normal_C|SetAnimLookAt (Variables|Default|GetPF_Normal) true)
      (Variables|Default|SetCanLMB true))
    (:OnInterrupted
      (goto _label))
    (:OnNotifyBegin
      (Networking|SwitchHasAuthority
        (:Authority
          (bind (_outhit _returnvalue_6) (Collision|BoxTraceByChannel _returnvalue_5 (+ _returnvalue_5 "0.000000,0.000000,-210.000000") "30.000000,15.000000,1.000000" (Transformation|GetActorRotation (Variables|Default|GetPF_Normal)) "TraceTypeQuery1" false 0 "None"))
          (if _returnvalue_6
            (bind _returnvalue_7 (Class|AdianFL|DoDamage (.HitActor (Collision|BreakHitResult _outhit)) (Utilities|Struct|MakeDamageInfo (Variables|Default|GetDA_DamageAction) (Variables|Default|GetPF_Normal) (.ImpactPoint (Collision|BreakHitResult _outhit)) 0.0)))
            (if _returnvalue_7
              (Class|DurabilityInterface|ApplyDurability(Message) (Variables|Default|GetPF_Normal) (Utilities|Struct|MakeApplyDurabilityIn "/Game/DataAssets/Durability/StandardDamage.StandardDamage" (Variables|Default|GetInventory) (Variables|Default|GetSlotIndex))))))))))

(event Custom|Server_Swing
  (CallFunction|MulticastSwing))

(event EventStartItemComponent
  (bind _pf_normal (Variables|Default|GetPF_Normal))
  (bind _abp_normal (Variables|/Game/Blueprints/PF_Normal.PF_Normal_C|GetABP_Normal _pf_normal))
  (Variables|/Game/Player/ABP_Normal.ABP_Normal_C|SetAnimArm_R _abp_normal "/Game/Player/Animations/Male_ITAN_Pickaxe.Male_ITAN_Pickaxe")
  (Variables|/Game/Player/ABP_Normal.ABP_Normal_C|SetAnimArm_L _abp_normal "/Game/Player/Animations/Male_ITAN_Pickaxe.Male_ITAN_Pickaxe")
  (Variables|/Game/Player/ABP_Normal.ABP_Normal_C|SetArm_R _abp_normal true)
  (Variables|/Game/Player/ABP_Normal.ABP_Normal_C|SetArm_R_Weight _abp_normal 1.0)
  (Variables|/Game/Player/ABP_Normal.ABP_Normal_C|SetArm_L _abp_normal true)
  (Variables|/Game/Player/ABP_Normal.ABP_Normal_C|SetArm_L_Weight _abp_normal 1.0)
  (bind _returnvalue (Game|AddComponentbyClass (Variables|Default|GetPF_Normal) "/Script/Engine.StaticMeshComponent" true (Math|Transform|MakeTransform "-7.500000,2.500000,0.000000" "0.000000,0.000000,-90.000000" "1.000000,1.000000,1.000000")))
  (bind _output_get (Variables|Default|SetStaticMeshComponent _returnvalue))
  (Utilities|FlowControl|Sequence
    (:then_0
      (bind _object (Utilities|AsyncLoadAsset (Utilities|Array|Get(acopy) (Utilities|Struct|BreakItemComponentParameters (Variables|/Script/SkyCraft.DA_Item|GetItemComponentParameters (Variables|Default|GetDA_Item)))))
        (:then
          (bind _returnvalue_2 (Utilities|LoadAssetBlocking (Utilities|Array|Get(acopy) (Utilities|Struct|BreakItemComponentParameters (Variables|/Script/SkyCraft.DA_Item|GetItemComponentParameters (Variables|Default|GetDA_Item))) 1)))
          (bind _asda_damage_action (Utilities|Casting|CastToDA_DamageAction _returnvalue_2))
          (Variables|Default|SetDA_DamageAction _asda_damage_action))
        (:Completed
          (bind _asstatic_mesh (Utilities|Casting|CastToStaticMesh _object))
          (Components|StaticMesh|SetStaticMesh _output_get _asstatic_mesh)
          (Class|AdianFL|ResolveStaticMeshCustomPrimitiveData (Variables|Default|GetStaticMeshComponent))
          (Transformation|AttachComponentToComponent (Variables|Default|GetStaticMeshComponent) (Variables|/Script/Engine.Character|GetMesh (Variables|Default|GetPF_Normal)) "RightHand" "KeepRelative" "KeepRelative" "KeepRelative" false))))
    (:then_1
      (if (CallFunction|IsLocallyControlled)
        (Actor|Tick|SetActorTickEnabled true)))))

(event EventLMB
  (params (Pressed :type Boolean))
  (Variables|Default|SetLMBPressed Pressed))

(event EventEndItemComponent
  (bind _pf_normal (Variables|Default|GetPF_Normal))
  (bind _pf_normal_2 (Variables|Default|GetPF_Normal))
  (bind _abp_normal (Variables|/Game/Blueprints/PF_Normal.PF_Normal_C|GetABP_Normal _pf_normal))
  (Variables|/Game/Player/ABP_Normal.ABP_Normal_C|SetArm_R _abp_normal false)
  (Variables|/Game/Player/ABP_Normal.ABP_Normal_C|SetArm_L _abp_normal false)
  (Variables|/Game/Blueprints/PF_Normal.PF_Normal_C|SetcanMove _pf_normal_2 true)
  (Variables|/Game/Blueprints/PF_Normal.PF_Normal_C|SetcanQSPressing _pf_normal_2 true)
  (Variables|/Game/Blueprints/PF_Normal.PF_Normal_C|SetAnimLookAt (Variables|Default|GetPF_Normal) true)
  (Class|AdianFL|ForceDestroyComponent (Variables|Default|GetStaticMeshComponent)))

(event EventTick
  (params (DeltaSeconds :type Float%20%28single-precision%29))
  (if (Math|Boolean|ANDBoolean (Variables|Default|GetCanLMB) (Variables|Default|GetLMBPressed) (not (AI|Components|NavMovement|IsFalling (Variables|/Script/Engine.Character|GetCharacterMovement (Variables|Default|GetPF_Normal)))))
    (Variables|Default|SetCanLMB false)
    (CallFunction|ServerSwing)))

(fn ConstructionScript)