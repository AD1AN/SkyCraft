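; Mattock item component that lets players raise or lower island terrain, or add grass and remove foliage.
; While equipped, it attaches the mesh and arm animations, and locally traces from the camera to place a color-coded preview, blocking terrain edits near resources.
; Cooldown-limited clicks send island-local positions to server events, which edit the Island and multicast montage, dust and sound.
; Alt toggles removal; right-click opens a widget, and editing mode persists in local settings.
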(event Custom|Server_FoliageAdd
  (params (Island :type Island%20Object%20Reference) (DA_Foliage :type DA%20Foliage%20Object%20Reference) (Location :type Vector%20Net%20Quantize%20Structure) (Radius :type Float%20%28single-precision%29))
  (Utilities|IsValid Island
    (:Is%20Valid
      (CallFunction|MulticastFoliageFX Island Location true)
      (Class|Island|FoliageAdd Island DA_Foliage Location Radius))))

(event Custom|Server_FoliageRemove
  (params (Island :type Island%20Object%20Reference) (Location :type Vector%20Net%20Quantize%20Structure) (Radius :type Float%20%28single-precision%29))
  (Utilities|IsValid Island
    (:Is%20Valid
      (CallFunction|MulticastFoliageFX Island Location false)
      (Class|Island|FoliageRemove Island Location Radius))))

(event Custom|Multicast_TerrainFX
  (params (Island :type Island%20Object%20Reference) (Location :type Vector%20Net%20Quantize%20Structure))
  (bind _rootcomponent (Variables|/Script/Engine.Actor|GetRootComponent Island))
  (Animation|Montage|PlayMontage (Variables|/Script/Engine.Character|GetMesh (Variables|Default|GetPF_Normal)) "/Game/Player/Animations/Male_Mattock_Foliage_Montage.Male_Mattock_Foliage_Montage"
    (:then
      (Niagara|SpawnSystemAttached "/Game/Niagara/NS_MattockDust.NS_MattockDust" _rootcomponent "None" Location "0, 0, 0" "KeepRelativeOffset" true)
      (Audio|SpawnSoundAttached "/Game/Audio/SFX/Mattock_Terrain.Mattock_Terrain" _rootcomponent "None" Location "0, 0, 0" "KeepRelativeOffset" false (Math|Random|RandomFloatinRange 1.0 1.5) (Math|Random|RandomFloatinRange 0.9 1.0) 0.0 "/Game/Audio/NormalAttenuation.NormalAttenuation" 0))))

(event Custom|SetEditingMode
  (params (EditingMode :type Boolean))
  (bind _output_get (Variables|Default|SetEditingMode EditingMode))
  (bind _output_get_2 (Variables|/Script/SkyCraft.LocalSettings|SetbMattockEditingMode (Variables|/Script/SkyCraft.GIS|GetLocalSettings (Variables|/Game/Blueprints/BP_GSS.BP_GSS_C|GetBP_GIS (Variables|Default|GetBP_GSS))) _output_get))
  (CallFunction|ServerSetEditingMode _output_get_2))

(event Custom|Server_SetEditingMode
  (params (EditingMode :type Boolean))
  (Variables|Default|SetEditingMode EditingMode))

(event Custom|Multicast_FoliageFX
  (params (Island :type Island%20Object%20Reference) (Location :type Vector%20Net%20Quantize%20Structure) (AddFoliage :type Boolean))
  (bind _rootcomponent (Variables|/Script/Engine.Actor|GetRootComponent Island))
  (Animation|Montage|PlayMontage (Variables|/Script/Engine.Character|GetMesh (Variables|Default|GetPF_Normal)) "/Game/Player/Animations/Male_Mattock_Foliage_Montage.Male_Mattock_Foliage_Montage"
    (:then
      (Niagara|SpawnSystemAttached "/Game/Niagara/NS_MattockDust.NS_MattockDust" _rootcomponent "None" Location "0, 0, 0" "KeepRelativeOffset" true)
      (Audio|SpawnSoundAttached "/Game/Audio/SFX/Mattock_RemoveFoliage.Mattock_RemoveFoliage" _rootcomponent "None" Location "0, 0, 0" "KeepRelativeOffset" false (Math|Random|RandomFloatinRange 1.0 1.5) (Math|Random|RandomFloatinRange 0.9 1.0) 0.0 "/Game/Audio/NormalAttenuation.NormalAttenuation" 0)
      (if AddFoliage
        (Audio|SpawnSoundAttached "/Game/Audio/SFX/Mattock_AddFoliage.Mattock_AddFoliage" _rootcomponent "None" Location "0, 0, 0" "KeepRelativeOffset" false (Math|Random|RandomFloatinRange 2.0 4.0) (Math|Random|RandomFloatinRange 0.8 1.0) 0.0 "/Game/Audio/NormalAttenuation.NormalAttenuation" 0)))))

(event Custom|Server_TerrainEdit
  (params (Island :type Island%20Object%20Reference) (Location :type Vector%20Net%20Quantize%20Structure) (Radius :type Float%20%28single-precision%29) (Strength :type Float%20%28single-precision%29))
  (Utilities|IsValid Island
    (:Is%20Valid
      (CallFunction|MulticastTerrainFX Island Location)
      (Class|Island|TerrainEdit Island Location Radius Strength)
      (Class|Island|FoliageRemove Island Location (+ Radius 5e+01)))))

(event EventAlt
  (params (Pressed :type Boolean))
  (if Pressed
    (Variables|Default|SetRemovalMode (not (Variables|Default|GetRemovalMode)))))

(event EventEndItemComponent
  (bind _pf_normal (Variables|Default|GetPF_Normal))
  (bind _mattockpreview (Variables|Default|GetMattockPreview))
  (bind _abp_normal (Variables|/Game/Blueprints/PF_Normal.PF_Normal_C|GetABP_Normal _pf_normal))
  (Variables|/Game/Player/ABP_Normal.ABP_Normal_C|SetArm_R _abp_normal false)
  (Variables|/Game/Player/ABP_Normal.ABP_Normal_C|SetArm_L _abp_normal false)
  (Utilities|FlowControl|Sequence
    (:then_0
      (Class|AdianFL|ForceDestroyComponent (Variables|Default|GetStaticMesh)))
    (:then_1
      (if (CallFunction|IsLocallyControlled)
        (Utilities|IsValid _mattockpreview
          (:Is%20Valid
            (Actor|DestroyActor _mattockpreview)))))))

(event EventTick
  (params (DeltaSeconds :type Float%20%28single-precision%29))
  (bind _mattockpreview (Variables|Default|GetMattockPreview))
  (bind _pf_normal (Variables|Default|GetPF_Normal))
  (bind _returnvalue (Transformation|GetActorLocation _mattockpreview))
  (bind _maincamera (Variables|/Game/Blueprints/PF_Normal.PF_Normal_C|GetMainCamera _pf_normal))
  (bind _returnvalue_2 (Transformation|GetWorldLocation _maincamera))
  (Variables|Default|SetResourceCollision false)
  (Utilities|FlowControl|Sequence
    (:then_0
      (if (< (Variables|Default|GetCurrentCooldown) (Variables|Default|GetMaxCooldown))
        (Variables|Default|SetCurrentCooldown (+ (Variables|Default|GetCurrentCooldown) (Utilities|Time|GetWorldDeltaSeconds)))))
    (:then_1
      (bind (_outhit _returnvalue_3) (Collision|LineTraceByChannel _returnvalue_2 (+ _returnvalue_2 (* (Math|Vector|GetForwardVector _maincamera) 4e+02) (* (Math|Vector|GetRightVector _maincamera) -5e+01)) "TraceTypeQuery4" false 0 "None"))
      (if _returnvalue_3
        (Transformation|SetActorLocation (Variables|Default|GetMattockPreview) (.Location (Collision|BreakHitResult _outhit)) false true)
        (Variables|Default|SetHitComponent (.HitComponent (Collision|BreakHitResult _outhit)))
        (Class|KismetSystemLibrary|IsObjectOfSoftClass (Variables|Default|GetHitComponent) "/Script/ProceduralMeshComponent.ProceduralMeshComponent" :!label _label
          (:True
            (bind _asisland (Utilities|Casting|CastToIsland (Components|GetOwner (Variables|Default|GetHitComponent)))
              (:then
                (Variables|Default|SetValidIsland _asisland)
                (if (Variables|Default|GetEditingMode)
                  (bind _outhits (Collision|MultiSphereTraceByChannel _returnvalue _returnvalue 2.5e+02 "TraceTypeQuery1" false 0 "None" false))
                  (bind _array_element (Utilities|Array|ForEachLoopwithBreak _outhits :!label _label_2)
                    (:LoopBody
                      (Class|KismetSystemLibrary|IsObjectOfSoftClass (.HitActor (Collision|BreakHitResult _array_element)) "/Script/SkyCraft.Resource"
                        (:True
                          (Variables|Default|SetResourceCollision true)
                          (goto _label_2 Break))))
                    (:Completed
                      (if (Variables|Default|GetResourceCollision)
                        (Rendering|Material|SetVectorParameterValueonMaterials (Variables|/Game/Blueprints/IC/MattockPreview.MattockPreview_C|GetSphere (Variables|Default|GetMattockPreview)) "BuildingPreviewColor" "0.500000,0.000000,0.000000" :!label _label_3)
                        (Variables|Default|SetValidIsland 0) ; Empty
                        (else
                          (Rendering|Material|SetVectorParameterValueonMaterials (Variables|/Game/Blueprints/IC/MattockPreview.MattockPreview_C|GetSphere (Variables|Default|GetMattockPreview)) "BuildingPreviewColor" (select (Variables|Default|GetRemovalMode) "1.000000,0.500000,0.250000" "0.000000,1.000000,0.000000") :!label _label_4)))))
                  (else
                    (goto _label_4))))
              (:CastFailed
                (goto _label_3))))
          (:False
            (goto _label_3)))
        (else
          (bind (_outhit_2 _returnvalue_4) (Collision|LineTraceByChannel (.TraceEnd (Collision|BreakHitResult _outhit)) (Math|Vector|MakeVector (.X (Math|Vector|BreakVector (.TraceEnd (Collision|BreakHitResult _outhit)))) (.Y (Math|Vector|BreakVector (.TraceEnd (Collision|BreakHitResult _outhit)))) (- (.z (Transformation|GetActorLocation (Variables|Default|GetPF_Normal))) 1.5e+02)) "TraceTypeQuery1" false 0 "None"))
          (if _returnvalue_4
            (Transformation|SetActorLocation (Variables|Default|GetMattockPreview) (.Location (Collision|BreakHitResult _outhit_2)) false true)
            (Variables|Default|SetHitComponent (.HitComponent (Collision|BreakHitResult _outhit_2)))
            (goto _label)
            (else
              (Transformation|SetActorLocation (Variables|Default|GetMattockPreview) (.TraceEnd (Collision|BreakHitResult _outhit_2)) false true)
              (goto _label_3))))))))

(event EventStartItemComponent
  (bind _pf_normal (Variables|Default|GetPF_Normal))
  (bind _abp_normal (Variables|/Game/Blueprints/PF_Normal.PF_Normal_C|GetABP_Normal _pf_normal))
  (Variables|/Game/Player/ABP_Normal.ABP_Normal_C|SetAnimArm_R _abp_normal "/Game/Player/Animations/Male_ITAN_Mattock.Male_ITAN_Mattock")
  (Variables|/Game/Player/ABP_Normal.ABP_Normal_C|SetAnimArm_L _abp_normal "/Game/Player/Animations/Male_ITAN_Mattock.Male_ITAN_Mattock")
  (Variables|/Game/Player/ABP_Normal.ABP_Normal_C|SetArm_R _abp_normal true)
  (Variables|/Game/Player/ABP_Normal.ABP_Normal_C|SetArm_R_Weight _abp_normal 1.0)
  (Variables|/Game/Player/ABP_Normal.ABP_Normal_C|SetArm_L _abp_normal true)
  (Variables|/Game/Player/ABP_Normal.ABP_Normal_C|SetArm_L_Weight _abp_normal 1.0)
  (Utilities|FlowControl|Sequence
    (:then_0
      (bind _returnvalue (Game|AddComponentbyClass (Variables|Default|GetPF_Normal) "/Script/Engine.StaticMeshComponent" true (Math|Transform|MakeTransform "-7.500000,2.500000,0.000000" "0.000000,0.000000,-90.000000" "1.000000,1.000000,1.000000")))
      (bind _output_get (Variables|Default|SetStaticMesh _returnvalue))
      (Components|StaticMesh|SetStaticMesh _output_get "/Game/s2u/StoneMattock.StoneMattock")
      (Class|AdianFL|ResolveStaticMeshCustomPrimitiveData (Variables|Default|GetStaticMesh))
      (Transformation|AttachComponentToComponent (Variables|Default|GetStaticMesh) (Variables|/Script/Engine.Character|GetMesh (Variables|Default|GetPF_Normal)) "RightHand" "KeepRelative" "KeepRelative" "KeepRelative" false))
    (:then_1
      (if (CallFunction|IsLocallyControlled)
        (bind _returnvalue_2 (Game|SpawnActorfromClass "/Game/Blueprints/IC/MattockPreview.MattockPreview_C" (Math|Transform|MakeTransform "0, 0, 0" "0, 0, 0" "1.000000,1.000000,1.000000") "AlwaysSpawn" "MultiplyWithRoot" 0 0))
        (Variables|Default|SetMattockPreview _returnvalue_2)
        (CallFunction|SetEditingMode (Variables|/Script/SkyCraft.LocalSettings|GetbMattockEditingMode (Variables|/Script/SkyCraft.GIS|GetLocalSettings (Variables|/Game/Blueprints/BP_GSS.BP_GSS_C|GetBP_GIS (Variables|Default|GetBP_GSS)))))
        (Actor|Tick|SetActorTickEnabled true)))))

(event EventRMB
  (params (Pressed :type Boolean))
  (if Pressed
    (Utilities|IsValid (Variables|Default|GetCWS_Mattock)
      (:Is%20Valid
        (if (not (UserInterface|Viewport|IsinViewport (Variables|Default|GetCWS_Mattock)))
          (UserInterface|Viewport|AddtoViewport (Variables|Default|GetCWS_Mattock) 25 :!label _label)
          (Default|AddCWS (Variables|Default|GetBP_PSS) (Variables|Default|GetCWS_Mattock) true true true "NewEnumerator2")))
      (:Is%20Not%20Valid
        (bind _returnvalue (UserInterface|CreateWidget "/Game/Widgets/CWS/CWS_Mattock.CWS_Mattock_C" 0 self))
        (Variables|Default|SetCWS_Mattock _returnvalue)
        (goto _label)))))

(event EventLMB
  (params (Pressed :type Boolean))
  (bind _validisland (Variables|Default|GetValidIsland))
  (bind _mattockpreview (Variables|Default|GetMattockPreview))
  (bind _validisland_2 (Variables|Default|GetValidIsland))
  (bind _validisland_3 (Variables|Default|GetValidIsland))
  (bind _returnvalue (Transformation|GetActorTransform _validisland_2))
  (bind _returnvalue_2 (Transformation|GetActorLocation _mattockpreview))
  (bind _returnvalue_3 (Math|Transform|InverseTransformLocation _returnvalue _returnvalue_2))
  (bind _returnvalue_4 (Math|Vector|MakeVectorNetQuantize (.x _returnvalue_3) (.y _returnvalue_3) (.z _returnvalue_3)))
  (if (Math|Boolean|ANDBoolean Pressed (Utilities|IsValid (Variables|Default|GetValidIsland)) (>= (Variables|Default|GetCurrentCooldown) (Variables|Default|GetMaxCooldown)))
    (Variables|Default|SetCurrentCooldown 0.0) ; reset to 0
    (if (Variables|Default|GetEditingMode)
      (if (Variables|Default|GetRemovalMode)
        (CallFunction|ServerTerrainEdit _validisland _returnvalue_4 2e+02 -5e+01)
        (else
          (CallFunction|ServerTerrainEdit _validisland _returnvalue_4 2e+02 5e+01)))
      (elif (Variables|Default|GetRemovalMode)
        (CallFunction|ServerFoliageRemove _validisland_3 _returnvalue_4 75.0)
        (else
          (CallFunction|ServerFoliageAdd _validisland_3 "/Game/DataAssets/Foliage/Grass1.Grass1" _returnvalue_4 5e+01))))))

(fn ConstructionScript)