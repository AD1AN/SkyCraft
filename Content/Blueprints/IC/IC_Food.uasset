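; IC_Food is an item component for edible food that the player eats with a left mouse press.
; The press calls a server event, which multicasts the eating montage and a randomly pitched, randomly loud attached eating sound.
; The server then subtracts hunger by the first float in the item parameters and consumes one item from the inventory slot.
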(event Custom|Multicast_Eat
  (Audio|SpawnSoundAttached "/Game/Audio/SFX/Eating.Eating" (Variables|/Script/Engine.Actor|GetRootComponent (Variables|Default|GetPF_Normal)) "None" "0, 0, 0" "0, 0, 0" "KeepRelativeOffset" false (Math|Random|RandomFloatinRange 0.8 1.3) (Math|Random|RandomFloatinRange 0.9 1.15) 0.0 "/Game/Audio/NormalAttenuation.NormalAttenuation" 0)
  (Animation|Montage|PlayMontage (Variables|/Script/Engine.Character|GetMesh (Variables|Default|GetPF_Normal)) "/Game/Player/Animations/Male_Eating_Montage.Male_Eating_Montage"))

(event Custom|Server_Eat
  (CallFunction|MulticastEat)
  (Class|HungerComponent|SubtractHunger (Variables|/Script/SkyCraft.PlayerNormal|GetHungerComponent (Variables|Default|GetPF_Normal)) (Utilities|Array|Get(acopy) (Utilities|Struct|BreakItemComponentParameters (Variables|Default|GetItemComponentParameters))))
  (Class|InventoryComponent|ConsumeSingle (Variables|/Script/SkyCraft.PlayerNormal|GetInventoryComponent (Variables|Default|GetPF_Normal)) (Variables|Default|GetSlotIndex)))

(event EventLMB
  (params (Pressed :type Boolean))
  (if Pressed
    (CallFunction|ServerEat)))

(fn ConstructionScript
  (|CallParentFunction))