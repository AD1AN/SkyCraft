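; A harvestable resource actor that gives random loot to the interacting pawn's inventory.
; BeginPlay configures mesh variety, material scalars, optional scale, sky tags and health from the DAResource data asset's size entry, restoring saved health when loaded.
; Server tap interaction rolls weighted loot, always from the first size entry, and destroys the actor on the first successful inventory add.
; A multicast event plays pitch-randomized sounds at its location.
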(event Custom|Multicast_PlaySound
  (params (Sound :type Sound%20Base%20Object%20Reference))
  (Audio|SpawnSoundatLocation Sound (Transformation|GetActorLocation) "0, 0, 0" 1.0 (Math|Random|RandomFloatinRange 0.75 1.2) 0.0 "/Game/Audio/SFX/NormalAttenuation.NormalAttenuation" 0))

(event EventBeginPlay
  (bind _da_resource (Variables|Default|GetDA_Resource))
  (bind _output_get (Variables|Default|SetCurrentSize (Utilities|Array|Get(acopy) (Variables|/Script/SkyCraft.DA_Resource|GetSize (Variables|Default|GetDA_Resource)) (Variables|Default|GetResourceSize))))
  (Components|StaticMesh|SetStaticMesh (Variables|Default|GetStaticMesh) (Utilities|Array|Get(acopy) (Utilities|Struct|BreakResourceSize _output_get) (Variables|Default|GetSM_Variety)))
  (Utilities|FlowControl|Sequence
    (:then_0
      (for _array_element (Variables|/Script/SkyCraft.DA_Resource|GetSkyTags (Variables|Default|GetDA_Resource))
        (Utilities|Array|Add (Variables|/Script/SkyCraft.SkyTags|GetDA_SkyTags (Variables|Default|GetSkyTags)) _array_element)))
    (:then_1
      (bind _output_get_2 (Variables|/Game/Blueprints/DamageSystem/DamageSystem.DamageSystem_C|SetMaxHealth_0 (Variables|Default|GetDamageSystem) (.Health (Utilities|Struct|BreakResourceSize (Variables|Default|GetCurrentSize)))))
      (Variables|/Game/Blueprints/DamageSystem/DamageSystem.DamageSystem_C|SetHealth_0 (Variables|Default|GetDamageSystem) (select (Variables|Default|GetLoaded) (Variables|Default|GetLoadHealth) _output_get_2)))
    (:then_2
      (for _array_element_2 (.SM_Scalar (Utilities|Struct|BreakResourceSize (Variables|Default|GetCurrentSize)))
        (Rendering|Material|SetScalarParameterforCustomPrimitiveData (Variables|Default|GetStaticMesh) (.ParameterName (Utilities|Struct|BreakSM_Scalar _array_element_2)) (.Value (Utilities|Struct|BreakSM_Scalar _array_element_2)))))
    (:then_3
      (if true
        (Variables|/Script/Engine.PrimitiveComponent|SetbGenerateOverlapEvents (Variables|Default|GetStaticMesh) true)
        (Variables|/Game/Blueprints/InteractSystem/InteractSystem_OLD.InteractSystem_OLD_C|SetInteractable (Variables|Default|GetInteractSystem) true)))
    (:then_4
      (if (Variables|/Script/SkyCraft.DA_Resource|GetChangeScale _da_resource)
        (Transformation|SetRelativeScale3D (Variables|Default|GetStaticMesh) (Variables|/Script/SkyCraft.DA_Resource|GetNewScale _da_resource))))))

(fn ConstructionScript)

(fn ClientInterrupt
  (params (InterruptedBy :type E_InterruptedBy_OLD%20Enum :default "NewEnumerator0") (InteractKey :type E_InteractKey_OLD%20Enum :default "NewEnumerator0") (InteractedPawn :type Pawn%20Object%20Reference) (InteractedPC_Sky :type PC%20Sky%20Object%20Reference) (InteractedPP_Sky :type PP%20Sky%20Object%20Reference))
  (return false))

(fn ClientTapInteract
  (params (InteractedKey :type E_InteractKey_OLD%20Enum :default "NewEnumerator0") (InteractedPawn :type Pawn%20Object%20Reference) (InteractedPC_Sky :type PC%20Sky%20Object%20Reference) (InteractedPP_Sky :type PP%20Sky%20Object%20Reference) (InteractedWith :type IC%20Class%20Reference))
  (return false))

(fn GetInteractLocation
  (return (Transformation|GetActorLocation)))

(fn GetInteractSystem
  (return (Variables|Default|GetInteractSystem)))

(fn GetSkyTags
  (return (Utilities|Struct|MakeGetSkyTagsOut (Variables|/Script/SkyCraft.SkyTags|GetDA_SkyTags (Variables|Default|GetSkyTags)))))

(fn ServerInterrupt
  (params (InterruptedBy :type E_InterruptedBy_OLD%20Enum :default "NewEnumerator0") (InteractKey :type E_InteractKey_OLD%20Enum :default "NewEnumerator0") (InteractedPawn :type Pawn%20Object%20Reference) (InteractedPC_Sky :type PC%20Sky%20Object%20Reference) (InteractedPP_Sky :type PP%20Sky%20Object%20Reference))
  (return false))

(fn ServerTapInteract
  (params (InteractedKey :type E_InteractKey_OLD%20Enum :default "NewEnumerator0") (InteractedPawn :type Pawn%20Object%20Reference) (InteractedPC_Sky :type PC%20Sky%20Object%20Reference) (InteractedPP_Sky :type PP%20Sky%20Object%20Reference) (InteractedWith :type IC%20Class%20Reference))
  (for _array_element (Utilities|Struct|BreakResourceSize (Utilities|Array|Get(acopy) (Variables|/Script/SkyCraft.DA_Resource|GetSize (Variables|Default|GetDA_Resource))))
    (if (Math|Random|RandomBoolwithWeight (.Probability (Utilities|Struct|BreakResourceLoot _array_element)))
      (bind _inventory (Class|BPIGeneral|GetInventory(Message) InteractedPawn))
      (bind _success (Default|AddtoInventory _inventory (Utilities|Struct|MakeInventorySlot (.Item (Utilities|Struct|BreakResourceLoot _array_element)) (Math|Random|RandomIntegerinRange (.Min (Utilities|Struct|BreakResourceLoot _array_element)) (.Max (Utilities|Struct|BreakResourceLoot _array_element))))))
      (if _success
        (Actor|DestroyActor)
        (return true)))))