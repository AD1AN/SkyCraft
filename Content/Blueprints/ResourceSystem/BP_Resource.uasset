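; BP_Resource is an interactable resource actor that grants loot from its DAResource data asset when used.
; ServerInteract rolls each loot entry of the first Size element by probability, sending a random quantity to the interacting pawn's inventory through an interface-style message.
; The first successful add destroys the actor and ends the loop, so one interaction yields at most one entry.
; A separate multicast event plays an attenuated sound at the actor with randomized pitch.
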(event Custom|Multicast_PlaySound
  (params (Sound :type Sound%20Base%20Object%20Reference))
  (Audio|SpawnSoundatLocation Sound (Transformation|GetActorLocation) "0, 0, 0" 1.0 (Math|Random|RandomFloatinRange 0.75 1.2) 0.0 "/Game/Audio/SFX/NormalAttenuation.NormalAttenuation" 0))

(fn ConstructionScript)

(fn ServerInteract
  (params (In :type Interact%20in%20Structure))
  (for _array_element (Utilities|Struct|BreakResourceSize (Utilities|Array|Get(acopy) (Variables|/Script/SkyCraft.DA_Resource|GetSize (Variables|Default|GetDA_Resource))))
    (if (Math|Random|RandomBoolwithWeight (.Probability (Utilities|Struct|BreakResourceLoot _array_element)))
      (bind _inventory (Class|BPIGeneral|GetInventory(Message) (.interactedpawn In)))
      (bind _success (Default|AddtoInventory _inventory (Utilities|Struct|MakeInventorySlot (.Item (Utilities|Struct|BreakResourceLoot _array_element)) (Math|Random|RandomIntegerinRange (.Min (Utilities|Struct|BreakResourceLoot _array_element)) (.Max (Utilities|Struct|BreakResourceLoot _array_element))))))
      (if _success
        (Actor|DestroyActor)
        (return (Utilities|Struct|MakeInteractOut true))))))