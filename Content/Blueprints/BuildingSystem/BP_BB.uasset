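; BP_BB is a building piece for the building system, with preview, outline and collision modes plus a stub placement check.
; Pieces form a Supports/Depends graph, recursively propagating Grounded (steps from ground), which also drives the preview color gradient.
; ServerDestroy refunds the data asset's required items, then re-evaluates supported pieces.
; Pieces exceeding GroundedMax are destroyed with refund, while those losing all Depends cascade-destroy without one.
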(fn ConstructionScript)

(fn PreviewMode
  (params (PreviewMode :type Boolean))
  (bind _returnvalue (Actor|GetComponentsByClass "/Script/Engine.StaticMeshComponent"))
  (if PreviewMode
    (for _array_element _returnvalue
      (Rendering|Material|SetMaterial _array_element 0 "/Game/GlobalMaterials/M_BuildingPreview.M_BuildingPreview"))
    (else
      (for (_array_element_2 _array_index) _returnvalue
        (Rendering|Material|SetMaterial _array_element_2 0 (Utilities|Array|Get(acopy) (Variables|Default|GetBBMaterials) _array_index))))))

(fn CollisionMode
  (params (CollisionMode :type ECollisionEnabled%20Enum :default "NoCollision"))
  (bind _returnvalue (Utilities|Select :Index CollisionMode :NoCollision false :QueryOnly false :PhysicsOnly true :QueryAndPhysics true))
  (Utilities|FlowControl|Sequence
    (:then_0
      (Collision|SetActorEnableCollision _returnvalue))
    (:then_1
      (for _array_element (Actor|GetAllChildActors false)
        (Collision|SetActorEnableCollision _array_element _returnvalue)))))

(fn OutlineMode
  (params (OutlineMode :type Boolean))
  (bind _returnvalue (Actor|GetComponentsByClass "/Script/Engine.StaticMeshComponent"))
  (if OutlineMode
    (for _array_element _returnvalue
      (Rendering|Material|SetMaterial _array_element 0 "/Game/GlobalMaterials/M_BuildingSelectOutline.M_BuildingSelectOutline"))
    (else
      (for (_array_element_2 _array_index) _returnvalue
        (Rendering|Material|SetMaterial _array_element_2 0 (Utilities|Array|Get(acopy) (Variables|Default|GetBBMaterials) _array_index))))))

(fn SetPreviewColor
  (params (ColorPreview :type E_BBPreviewColor%20Enum :default "NewEnumerator0"))
  (bind _returnvalue (Math|Vector|MakeVector 0.1 0.1 1.0))
  (bind _returnvalue_2 (Actor|GetComponentsByClass "/Script/Engine.StaticMeshComponent"))
  (bind _grounded (Variables|Default|GetGrounded))
  (bind _groundedmax (Variables|Default|GetGroundedMax))
  (bind _returnvalue_3 (Math|Conversions|ToFloat(Byte) _groundedmax))
  (bind _returnvalue_4 (Math|Conversions|ToFloat(Byte) _grounded))
  (bind _returnvalue_5 (Math|Float|MapRangeClamped _returnvalue_4 0.0 _returnvalue_3 1.0 0.25))
  (bind _returnvalue_6 (Math|Float|MapRangeClamped _returnvalue_4 0.0 _returnvalue_3 0.0 0.85))
  (switch Utilities|FlowControl|Switch|SwitchonE_BBPreviewColor ColorPreview
    (:NewEnumerator0
      (for _array_element _returnvalue_2
        (Rendering|Material|SetVectorParameterValueonMaterials _array_element "BuildingPreviewColor" "1.000000, 0, 0")))
    (:NewEnumerator1
      (for _array_element_2 _returnvalue_2
        (Rendering|Material|SetVectorParameterValueonMaterials _array_element_2 "BuildingPreviewColor" _returnvalue)))
    (:NewEnumerator2
      (for _array_element_3 _returnvalue_2
        (Rendering|Material|SetVectorParameterValueonMaterials _array_element_3 "BuildingPreviewColor" (Math|Vector|MakeVector _returnvalue_6 _returnvalue_5 0.0))))
    (:NewEnumerator3
      (for _array_element_4 _returnvalue_2
        (Rendering|Material|SetVectorParameterValueonMaterials _array_element_4 "BuildingPreviewColor" (select (> _grounded 0) (Math|Vector|MakeVector _returnvalue_6 _returnvalue_5 0.0) _returnvalue))))))

(fn CheckPlacing
  (return false 0 false))

(fn UpdateGroundedonBuild
  (params (NewGrounded :type Byte))
  (Variables|Default|SetGrounded NewGrounded)
  (for _array_element (Variables|Default|GetSupports)
    (if (not (<= (Variables|/Script/SkyCraft.BB|GetGrounded _array_element) (+ 1 (Variables|Default|GetGrounded))))
      (bind _asbp_bb (Utilities|Casting|CastToBP_BB _array_element))
      (CallFunction|UpdateGroundedonBuild _asbp_bb (+ 1 (Variables|Default|GetGrounded))))))

(fn UpdateGroundedonDestroy
  (params (NewGrounded :type Byte) (PlayerObject :type Object%20Object%20Reference))
  (bind _output_get (Variables|Default|SetGrounded NewGrounded))
  (if (> _output_get (Variables|Default|GetGroundedMax))
    (CallFunction|ServerDestroy PlayerObject)
    (else
      (for _array_element (Variables|Default|GetSupports)
        (bind _lowestgrounded (CallFunction|LowestGrounded (Variables|/Script/SkyCraft.BB|GetDepends _array_element)))
        (if (!= _lowestgrounded (Variables|/Script/SkyCraft.BB|GetGrounded _array_element))
          (bind _asbp_bb (Utilities|Casting|CastToBP_BB _array_element))
          (CallFunction|UpdateGroundedonDestroy _asbp_bb _lowestgrounded PlayerObject))))))

(fn LowestGrounded
  (params (BA :type Array%20of%20BB%20Object%20References))
  (for _array_element BA
    (if (or (< (+ (Variables|/Script/SkyCraft.BB|GetGrounded _array_element) 1) (LocalVariables|Get_LowestGrounded)) (< (LocalVariables|Get_LowestGrounded) 1))
      (LocalVariables|Set_LowestGrounded (+ (Variables|/Script/SkyCraft.BB|GetGrounded _array_element) 1))))
  (return (LocalVariables|Get_LowestGrounded)))

(fn AddOffsettoActor
  (params (Offset :type Vector))
  (bind _defaultsceneroot (Variables|Default|GetDefaultSceneRoot))
  (return (+ (Transformation|GetActorLocation) (* (Math|Vector|GetForwardVector _defaultsceneroot) (.x Offset)) (* (Math|Vector|GetRightVector _defaultsceneroot) (.y Offset)) (* (Math|Vector|GetUpVector _defaultsceneroot) (.z Offset)))))

(fn ZeroDependsDestroy
  (for _array_element (Variables|Default|GetSupports)
    (Utilities|Array|RemoveItem (Variables|/Script/SkyCraft.BB|GetDepends _array_element) self)
    (if (<= (Utilities|Array|Length (Variables|/Script/SkyCraft.BB|GetDepends _array_element)) 0)
      (bind _asbp_bb (Utilities|Casting|CastToBP_BB _array_element))
      (CallFunction|ZeroDependsDestroy _asbp_bb)))
  (Actor|DestroyActor))

(fn ServerDestroy
  (params (PlayerObject :type Object%20Object%20Reference))
  (bind _da_bb (Variables|Default|GetDA_BB))
  (bind _inventory (Class|BPIGetInventory|GetInventory(Message) PlayerObject))
  (Utilities|IsValid _da_bb
    (:Is%20Valid
      (for _array_element (Variables|/Script/SkyCraft.DA_BB|GetRequiredItems _da_bb)
        (bind _success (Default|AddtoInventory _inventory _array_element))
        (if _success
          _)))
    (:Is%20Not%20Valid
      (CallFunction|AdianPrintError (Utilities|String|Append "BUILDING ROW IS CORRUPTED: " (Utilities|GetDisplayName self)))))
  (Utilities|FlowControl|Sequence
    (:then_0
      (for _array_element_2 (Variables|Default|GetSupports)
        (Utilities|Array|RemoveItem (Variables|/Script/SkyCraft.BB|GetDepends _array_element_2) self)
        (bind _asbp_bb (Utilities|Casting|CastToBP_BB _array_element_2)
          (:then
            _)
          (:CastFailed
            _))
        (if (<= (Utilities|Array|Length (Variables|/Script/SkyCraft.BB|GetDepends _array_element_2)) 0)
          (CallFunction|ZeroDependsDestroy _asbp_bb)
          (else
            (bind _lowestgrounded (CallFunction|LowestGrounded _asbp_bb (Variables|/Script/SkyCraft.BB|GetDepends _array_element_2)))
            (CallFunction|UpdateGroundedonDestroy _asbp_bb _lowestgrounded PlayerObject)))))
    (:then_1
      (Utilities|FlowControl|Sequence
        (:then_0
          (for _array_element_3 (Variables|Default|GetDepends)
            (Utilities|Array|RemoveItem (Variables|/Script/SkyCraft.BB|GetSupports _array_element_3) self)))
        (:then_1
          (Actor|DestroyActor))))))