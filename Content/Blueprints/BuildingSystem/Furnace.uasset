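; Placeable furnace building that burns fuel to cook input items into output items, with a UI widget opened on interact.
; Changes to fuel or input slots run TryCook, which matches items against fuel and recipe DataTables and starts burning.
; Tick consumes fuel, advances or rewinds cook progress and updates inventories through multicasts.
; It also overrides building placement traces and save/load of transform and slots.
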(event Custom|SAE_Inventory_Fuel
  (params (SlotIndex :type Integer))
  (CallFunction|TryCook))

(event Custom|SAE_Inventory_Input
  (params (SlotIndex :type Integer))
  (CallFunction|TryCook))

(event Custom|Uncook
  (Variables|Default|SetCurrentCookTime (Math|Float|Clamp(Float) (- (Variables|Default|GetCurrentCookTime) (Utilities|Time|GetWorldDeltaSeconds)) 0.0 (Variables|Default|GetEndCookTime))) ; Uncook
)

(event EventBeginPlay
  (EventDispatchers|BindEventtoOnChangeSlot (Variables|Default|GetInventoryFuel) (delegate Custom|SAE_Inventory_Fuel))
  (EventDispatchers|BindEventtoOnChangeSlot (Variables|Default|GetInventoryInput) (delegate Custom|SAE_Inventory_Input)))

(event EventTick
  (params (DeltaSeconds :type Float%20%28single-precision%29))
  (bind _inventoryfuel (Variables|Default|GetInventoryFuel))
  (bind _fuel (Variables|Default|GetFuel))
  (bind _inventoryinput (Variables|Default|GetInventoryInput))
  (bind _output (Variables|Default|GetOutput))
  (bind _fuel_2 (Variables|Default|GetFuel))
  (bind _output_2 (Utilities|Struct|BreakS_FurnaceOutput _output))
  (bind _fuel_3 (Utilities|Struct|BreakS_FurnaceFuel _fuel_2))
  (bind _slots (Variables|/Script/SkyCraft.Inventory|GetSlots _inventoryinput))
  (bind _slots_2 (Variables|/Script/SkyCraft.Inventory|GetSlots _inventoryfuel))
  (bind _quantity (Utilities|Struct|BreakSlot _fuel_3))
  (bind _da_item (Utilities|Struct|BreakSlot _output_2))
  (bind _output_3 (Utilities|Array|Get(acopy) _slots_2))
  (bind _output_4 (Utilities|Array|Get(acopy) _slots))
  (bind _quantity_2 (Utilities|Struct|BreakSlot _output_3))
  (if (> (Variables|Default|GetCurrentFuelTime) 0.0) ; Have fuel?
    (Variables|Default|SetCurrentFuelTime (- (Variables|Default|GetCurrentFuelTime) (Utilities|Time|GetWorldDeltaSeconds))) ; Burn fuel
    (Utilities|FlowControl|Sequence
      (:then_0
        (Utilities|IsValid (Utilities|Struct|BreakSlot (Utilities|Array|Get(acopy) (Variables|/Script/SkyCraft.Inventory|GetSlots (Variables|Default|GetInventoryInput))))
          (:Is%20Valid
            (Variables|Default|SetCurrentCookTime (+ (Variables|Default|GetCurrentCookTime) (Utilities|Time|GetWorldDeltaSeconds))) ; Cooking
          )
          (:Is%20Not%20Valid
            (Variables|Default|SetCurrentCookTime (Math|Float|Clamp(Float) (- (Variables|Default|GetCurrentCookTime) (Utilities|Time|GetWorldDeltaSeconds)) 0.0 (Variables|Default|GetEndCookTime))) ; Uncook
          )))
      (:then_1
        (if (>= (Variables|Default|GetCurrentCookTime) (Variables|Default|GetEndCookTime)) ; COOKED?
          (bind _structout (Utilities|Struct|SetmembersinSlot _output_4 (- (Utilities|Struct|BreakSlot _output_4) 1)))
          (Class|Inventory|MulticastChangeSlot (Variables|Default|GetInventoryInput) 0 _structout)
          (Utilities|IsValid _da_item
            (:Is%20Valid
              (Utilities|FlowControl|Sequence
                (:then_0
                  (if (Variables|/Script/SkyCraft.DA_Item|GetbCanStack _da_item)
                    _
                    (else
                      (Class|Inventory|MulticastEmptySlot (Variables|Default|GetInventoryOutput))))
                  (Class|Inventory|InsertSlot (Variables|Default|GetInventoryOutput) (.Output (Utilities|Struct|BreakS_FurnaceOutput (Variables|Default|GetOutput)))))
                (:then_1
                  (Variables|Default|SetCurrentCookTime 0.0))))
            (:Is%20Not%20Valid
              (CallFunction|AdianPrintError "ERROR: IDK WTF I JUST COOKED")))))
      (:then_2
        (if (<= (Variables|Default|GetCurrentFuelTime) 0.0) ; Fuel burnt out
          (Variables|Default|SetCurrentFuelTime 0.0)
          (Utilities|IsValid (.da_item (Utilities|Array|Get(acopy) (Variables|/Script/SkyCraft.Inventory|GetSlots (Variables|Default|GetInventoryInput))))
            (:Is%20Valid
              (if (>= _quantity_2 _quantity)
                (bind _structout_2 (Utilities|Struct|SetmembersinSlot _output_3 (- _quantity_2 _quantity)))
                (Class|Inventory|MulticastChangeSlot (Variables|Default|GetInventoryFuel) 0 _structout_2)
                (Variables|Default|SetCurrentFuelTime (.fueltime _fuel))
                (Variables|Default|SetMaxFuelTime (.fueltime _fuel))
                (Variables|Default|SetFuelEfficiency (.fuelefficiency _fuel))))))))
    (else
      (CallFunction|Uncook))))

(fn ConstructionScript)

(fn TryCook
  (bind _inventoryfuel (Variables|Default|GetInventoryFuel))
  (bind _slots (Variables|/Script/SkyCraft.Inventory|GetSlots _inventoryfuel))
  (bind _output (Utilities|Array|Get(acopy) _slots))
  (Utilities|FlowControl|Sequence
    (:then_0
      (Utilities|IsValid (.da_item (Utilities|Array|Get(acopy) (Variables|/Script/SkyCraft.Inventory|GetSlots (Variables|Default|GetInventoryFuel))))
        (:Is%20Valid
          (bind _outrownames (DataTable|GetDataTableRowNames "/Game/Blueprints/BuildingSystem/Furnace/DT_FurnaceFuel.DT_FurnaceFuel"))
          (bind _array_element (Utilities|Array|ForEachLoopwithBreak _outrownames :!label _label)
            (:LoopBody
              (bind _returnvalue (Utilities|GetDataTableRow "/Game/Blueprints/BuildingSystem/Furnace/DT_FurnaceFuel.DT_FurnaceFuel" _array_element)
                (:then
                  (Variables|Default|SetFuel _returnvalue)
                  (if (== (Utilities|Struct|BreakSlot (Utilities|Struct|BreakS_FurnaceFuel _returnvalue)) (.da_item (Utilities|Array|Get(acopy) (Variables|/Script/SkyCraft.Inventory|GetSlots (Variables|Default|GetInventoryFuel)))))
                    (LocalVariables|SetFuelFound true)
                    (goto _label Break)))))))
        (:Is%20Not%20Valid
          (return))))
    (:then_1
      (if (LocalVariables|GetFuelFound)
        (Utilities|IsValid (.da_item (Utilities|Array|Get(acopy) (Variables|/Script/SkyCraft.Inventory|GetSlots (Variables|Default|GetInventoryInput))))
          (:Is%20Valid
            (bind _outrownames_2 (DataTable|GetDataTableRowNames "/Game/Blueprints/BuildingSystem/Furnace/DT_FurnaceOutput.DT_FurnaceOutput"))
            (bind _array_element_2 (Utilities|Array|ForEachLoopwithBreak _outrownames_2 :!label _label_2)
              (:LoopBody
                (bind _returnvalue_2 (Utilities|GetDataTableRow "/Game/Blueprints/BuildingSystem/Furnace/DT_FurnaceOutput.DT_FurnaceOutput" _array_element_2)
                  (:then
                    (Variables|Default|SetOutput _returnvalue_2)
                    (if (== (.DA_Item (Utilities|Struct|BreakSlot (.Input (Utilities|Struct|BreakS_FurnaceOutput _returnvalue_2)))) (.da_item (Utilities|Array|Get(acopy) (Variables|/Script/SkyCraft.Inventory|GetSlots (Variables|Default|GetInventoryInput)))))
                      (LocalVariables|SetOutputFound true)
                      (goto _label_2 Break)))))))
          (:Is%20Not%20Valid
            (return)))
        (else
          (return))))
    (:then_2
      (if (and (LocalVariables|GetFuelFound) (LocalVariables|GetOutputFound))
        (Utilities|FlowControl|Sequence
          (:then_0
            (if (not (> (Variables|Default|GetCurrentFuelTime) 0.0))
              (Variables|Default|SetCurrentFuelTime (.FuelTime (Utilities|Struct|BreakS_FurnaceFuel (Variables|Default|GetFuel))))
              (if (<= (- (Utilities|Struct|BreakSlot (Utilities|Array|Get(acopy) (Variables|/Script/SkyCraft.Inventory|GetSlots (Variables|Default|GetInventoryFuel)))) (Utilities|Struct|BreakSlot (.Fuel (Utilities|Struct|BreakS_FurnaceFuel (Variables|Default|GetFuel))))) 0)
                (Class|Inventory|MulticastEmptySlot (Variables|Default|GetInventoryFuel))
                (else
                  (Class|Inventory|MulticastChangeSlot (Variables|Default|GetInventoryFuel) 0 (Utilities|Struct|MakeSlot (.da_item _output) (- (Utilities|Struct|BreakSlot (Utilities|Array|Get(acopy) (Variables|/Script/SkyCraft.Inventory|GetSlots (Variables|Default|GetInventoryFuel)))) (Utilities|Struct|BreakSlot (.Fuel (Utilities|Struct|BreakS_FurnaceFuel (Variables|Default|GetFuel))))) (.properties _output)))))))
          (:then_1
            (Variables|Default|SetFuelEfficiency (.FuelEfficiency (Utilities|Struct|BreakS_FurnaceFuel (Variables|Default|GetFuel))))
            (Variables|Default|SetMaxFuelTime (.FuelTime (Utilities|Struct|BreakS_FurnaceFuel (Variables|Default|GetFuel))))
            (Variables|Default|SetEndCookTime (.CookTime (Utilities|Struct|BreakS_FurnaceOutput (Variables|Default|GetOutput))))))
        (else
          (return))))))

(fn SaveBuildingParameters
  (bind _defaultsceneroot (Variables|Default|GetDefaultSceneRoot))
  (return (Utilities|Struct|MakeBuildingParameters (Utilities|Array|MakeArray (Variables|/Script/Engine.SceneComponent|GetRelativeLocation _defaultsceneroot)) (Utilities|Array|MakeArray (Variables|/Script/Engine.SceneComponent|GetRelativeRotation _defaultsceneroot)) (Utilities|Array|MakeArray (Utilities|Struct|MakeArrayInventorySlots (Variables|/Script/SkyCraft.Inventory|GetSlots (Variables|Default|GetInventoryInput))) (Utilities|Struct|MakeArrayInventorySlots (Variables|/Script/SkyCraft.Inventory|GetSlots (Variables|Default|GetInventoryOutput))) (Utilities|Struct|MakeArrayInventorySlots (Variables|/Script/SkyCraft.Inventory|GetSlots (Variables|Default|GetInventoryFuel)))))))

(fn LoadBuildingParameters
  (params (BuildingParameters :type Building%20Parameters%20Structure))
  (bind (_vectors _rotations _arrayinventoryslots) (Utilities|Struct|BreakBuildingParameters BuildingParameters))
  (Transformation|SetRelativeLocationAndRotation (Variables|Default|GetDefaultSceneRoot) (Utilities|Array|Get(acopy) _vectors) (Utilities|Array|Get(acopy) _rotations) false true)
  (for (_array_element _array_index) _arrayinventoryslots
    (Variables|/Script/SkyCraft.Inventory|SetSlots (Utilities|Select :Index _array_index :Option%200 (Variables|Default|GetInventoryInput) :Option%201 (Variables|Default|GetInventoryOutput) :Option%202 (Variables|Default|GetInventoryFuel)) (Utilities|Struct|BreakArrayInventorySlots _array_element))
    (return true)))

(fn CornersLinetraces
  (params (Dimensions :type Vector%202D%20Structure) (Debug :type Boolean))
  (bind (_valid _uniquefloors) (|CallParentFunction "(X=70.000000,Y=70.000000)" Debug))
  (return _valid _uniquefloors))

(fn CheckFreeBuildingPlacing
  (bind _returnvalue (Transformation|GetActorLocation))
  (bind (_valid _uniquefloors) (CallFunction|FreeBuildingLinetraces false))
  (if _valid
    (bind _returnvalue_2 (Collision|BoxTraceByChannel (+ _returnvalue "0,0,6.000000") (+ _returnvalue "0.000000,0.000000,70.000000") "40.000000,40.000000,1.000000" (Transformation|GetActorRotation) "TraceTypeQuery1" false 0 "None" true "(R=1.000000,G=0.000000,B=0.000000,A=1.000000)" "(R=0.000000,G=1.000000,B=0.000000,A=1.000000)" 2.0))
    (if (not _returnvalue_2)
      (return true (Utilities|Array|Get(acopy) _uniquefloors))
      (else
        (return false 0)))))

(fn ClientInteractBP
  (params (InteractKey :type EInteractKey%20Enum :default "Interact1") (Pawn :type Pawn%20Object%20Reference) (BP_PAI :type BP%20PAI%20Object%20Reference))
  (switch Utilities|FlowControl|Switch|SwitchonEInteractKey InteractKey
    (:Interact1
      (bind _returnvalue (UserInterface|CreateWidget "/Game/Widgets/CWS/CWS_Furnace.CWS_Furnace_C" 0 self Pawn))
      (UserInterface|Viewport|AddtoViewport _returnvalue 0)
      (Default|AddCWS BP_PAI _returnvalue true true "NewEnumerator2")
      (Default|SetMousetoCenter BP_PAI)
      (return true))))

(fn ClientInterruptBP
  (params (InterruptedBy :type EInterruptedBy%20Enum :default "Player") (InteractKey :type EInteractKey%20Enum :default "Interact1") (Pawn :type Pawn%20Object%20Reference) (BP_PAI :type BP%20PAI%20Object%20Reference))
  (return false))

(fn ServerInteractBP
  (params (InteractKey :type EInteractKey%20Enum :default "Interact1") (Pawn :type Pawn%20Object%20Reference) (BP_PAI :type BP%20PAI%20Object%20Reference))
  (return false))

(fn ServerInterruptBP
  (params (InterruptedBy :type EInterruptedBy%20Enum :default "Player") (InteractKey :type EInteractKey%20Enum :default "Interact1") (Pawn :type Pawn%20Object%20Reference) (BP_PAI :type BP%20PAI%20Object%20Reference))
  (return false))