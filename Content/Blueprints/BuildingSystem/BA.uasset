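; Base building-piece actor for the building system, handling preview, editing, structural support and destruction, with a stub placement check.
; Caches mesh materials to swap between preview, outline and original looks, tinting previews by state or Grounded value.
; Depends and Supports links form a support graph that propagates Grounded, a step count from the ground.
; Destruction refunds required items from the data table and cascades to pieces left unsupported or beyond GroundedMax.
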(event EventBeginPlay
  (for _array_element (Actor|GetComponentsByClass "/Script/Engine.StaticMeshComponent")
    (Utilities|Array|Add (Variables|Default|GetBuildingMaterials) (Rendering|Material|GetMaterial _array_element 0))))

(fn ConstructionScript)

(fn PreviewMode
  (params (PreviewMode :type Boolean))
  (bind _returnvalue (Actor|GetComponentsByClass "/Script/Engine.StaticMeshComponent"))
  (if PreviewMode
    (for _array_element _returnvalue
      (Rendering|Material|SetMaterial _array_element 0 "/Game/GlobalMaterials/M_BuildingPreview.M_BuildingPreview"))
    (else
      (for (_array_element_2 _array_index) _returnvalue
        (Rendering|Material|SetMaterial _array_element_2 0 (Utilities|Array|Get(acopy) (Variables|Default|GetBuildingMaterials) _array_index))))))

(fn CollisionMode
  (params (CollisionMode :type ECollisionEnabled%20Enum :default "NoCollision"))
  (bind _returnvalue (Utilities|Select :Index CollisionMode :NoCollision false :QueryOnly false :PhysicsOnly true :QueryAndPhysics true))
  (Utilities|FlowControl|Sequence
    (:then_0
      (Collision|SetActorEnableCollision _returnvalue))
    (:then_1
      (for _array_element (Actor|GetAllChildActors false)
        (Collision|SetActorEnableCollision _array_element _returnvalue)))))

(fn EditRotation
  (params (Up :type Boolean))
  (bind _returnvalue (Transformation|GetActorRotation))
  (bind _returnvalue_2 (Transformation|GetActorRotation))
  (if Up
    (Transformation|SetActorRotation (Math|Rotator|MakeRotator (.roll _returnvalue_2) (.pitch _returnvalue_2) (+ (.yaw _returnvalue_2) (Variables|Default|GetBuildingRotation))))
    (else
      (Transformation|SetActorRotation (Math|Rotator|MakeRotator (.roll _returnvalue) (.pitch _returnvalue) (- (.yaw _returnvalue) (Variables|Default|GetBuildingRotation)))))))

(fn ApplyEdit
  (Modes|PreviewMode false)
  (Widget|RemovefromParent (Variables|Default|GetW_EditMode))
  (Variables|Default|SetW_EditMode 0))

(fn DiscardEdit
  (bind _returnvalue (Transformation|GetActorRotation))
  (Transformation|SetActorRotation (Math|Rotator|MakeRotator (.roll _returnvalue) (.pitch _returnvalue) 0.0))
  (Modes|PreviewMode false)
  (Widget|RemovefromParent (Variables|Default|GetW_EditMode))
  (Variables|Default|SetW_EditMode 0))

(fn SetPreviewColor
  (params (ColorPreview :type E_PreviewColor%20Enum :default "NewEnumerator0"))
  (bind _returnvalue (Math|Vector|MakeVector 0.1 0.1 1.0))
  (bind _returnvalue_2 (Actor|GetComponentsByClass "/Script/Engine.StaticMeshComponent"))
  (bind _grounded (Variables|Stats|GetGrounded))
  (bind _groundedmax (Variables|Stats|GetGroundedMax))
  (bind _returnvalue_3 (Math|Conversions|ToFloat(Integer) _groundedmax))
  (bind _returnvalue_4 (Math|Conversions|ToFloat(Integer) _grounded))
  (bind _returnvalue_5 (Math|Float|MapRangeClamped _returnvalue_4 0.0 _returnvalue_3 1.0 0.25))
  (bind _returnvalue_6 (Math|Float|MapRangeClamped _returnvalue_4 0.0 _returnvalue_3 0.0 0.85))
  (switch Utilities|FlowControl|Switch|SwitchonE_PreviewColor ColorPreview
    (:NewEnumerator0
      (for _array_element _returnvalue_2
        (Rendering|Material|SetVectorParameterValueonMaterials _array_element "BuildingPreviewColor" "1.000000, 0, 0")))
    (:NewEnumerator1
      (for _array_element_2 _returnvalue_2
        (Rendering|Material|SetVectorParameterValueonMaterials _array_element_2 "BuildingPreviewColor" _returnvalue)))
    (:NewEnumerator2
      (for _array_element_3 _returnvalue_2
        (Rendering|Material|SetVectorParameterValueonMaterials _array_element_3 "BuildingPreviewColor" (Math|Vector|MakeVector _returnvalue_6 _returnvalue_5 0.0))))
    (:NewEnumerator3
      (for _array_element_4 _returnvalue_2
        (Rendering|Material|SetVectorParameterValueonMaterials _array_element_4 "BuildingPreviewColor" (select (> _grounded 0) (Math|Vector|MakeVector _returnvalue_6 _returnvalue_5 0.0) _returnvalue))))))

(fn AddOffsettoActor
  (params (Offset :type Vector))
  (bind _scene (Variables|Default|GetScene))
  (return (+ (Transformation|GetActorLocation) (* (Math|Vector|GetForwardVector _scene) (.x Offset)) (* (Math|Vector|GetRightVector _scene) (.y Offset)) (* (Math|Vector|GetUpVector _scene) (.z Offset)))))

(fn CheckPlacing
  (return false 0 false))

(fn ZeroDependsDestroy
  (for _array_element (Variables|ConnectionBuildings|GetSupports)
    (Utilities|Array|RemoveItem (Variables|BA_C|GetDepends _array_element) self)
    (if (<= (Utilities|Array|Length (Variables|BA_C|GetDepends _array_element)) 0)
      (CallFunction|ZeroDependsDestroy _array_element)))
  (Actor|DestroyActor))

(fn ServerDestroy
  (params (PlayerObject :type Object%20Object%20Reference))
  (bind _buildingrow (Variables|Default|GetBuildingRow))
  (bind _inventory (Class|BPIGeneral|GetInventory(Message) PlayerObject))
  (bind _returnvalue (Utilities|GetDataTableRow (.datatable _buildingrow) (.rowname _buildingrow))
    (:then
      (for _array_element (Utilities|Struct|BreakS_Building _returnvalue)
        (bind _success (Default|AddtoInventory _inventory _array_element))
        (if _success
          _)))
    (:RowNotFound
      (CallFunction|A1PrintError (Utilities|String|Append "BUILDING ROW IS CORRUPTED: " (Utilities|GetDisplayName self)))))
  (Utilities|FlowControl|Sequence
    (:then_0
      (for _array_element_2 (Variables|ConnectionBuildings|GetSupports)
        (Utilities|Array|RemoveItem (Variables|BA_C|GetDepends _array_element_2) self)
        (if (<= (Utilities|Array|Length (Variables|BA_C|GetDepends _array_element_2)) 0)
          (CallFunction|ZeroDependsDestroy _array_element_2)
          (else
            (bind _lowestgrounded (CallFunction|LowestGrounded _array_element_2 (Variables|BA_C|GetDepends _array_element_2)))
            (CallFunction|UpdateGroundedonDestroy _array_element_2 _lowestgrounded PlayerObject)))))
    (:then_1
      (Utilities|FlowControl|Sequence
        (:then_0
          (for _array_element_3 (Variables|ConnectionBuildings|GetDepends)
            (Utilities|Array|RemoveItem (Variables|BA_C|GetSupports _array_element_3) self)))
        (:then_1
          (Actor|DestroyActor))))))

(fn StartEditing
  (params (self2 :type PC%20Sky%20Object%20Reference) (InteractedPawn :type Pawn%20Object%20Reference))
  (bind _returnvalue (UserInterface|CreateWidget "/Game/Widgets/W_EditMode.W_EditMode_C" 0 self (Variables|/Game/Blueprints/PC_Sky.PC_Sky_C|GetPF_Normal self2)))
  (bind _output_get (Variables|Default|SetW_EditMode _returnvalue))
  (UserInterface|Viewport|AddtoViewport _output_get 0)
  (Modes|PreviewMode true))

(fn UpdateGroundedonBuild
  (params (NewGrounded :type Integer))
  (Variables|Stats|SetGrounded NewGrounded)
  (for _array_element (Variables|ConnectionBuildings|GetSupports)
    (if (not (<= (Variables|BA_C|GetGrounded _array_element) (+ 1 (Variables|Stats|GetGrounded))))
      (CallFunction|UpdateGroundedonBuild _array_element (+ 1 (Variables|Stats|GetGrounded))))))

(fn UpdateGroundedonDestroy
  (params (NewGrounded :type Integer) (PlayerObject :type Object%20Object%20Reference))
  (bind _output_get (Variables|Stats|SetGrounded NewGrounded))
  (if (> _output_get (Variables|Stats|GetGroundedMax))
    (CallFunction|ServerDestroy PlayerObject)
    (else
      (for _array_element (Variables|ConnectionBuildings|GetSupports)
        (bind _lowestgrounded (CallFunction|LowestGrounded _array_element (Variables|BA_C|GetDepends _array_element)))
        (if (!= _lowestgrounded (Variables|BA_C|GetGrounded _array_element))
          (CallFunction|UpdateGroundedonDestroy _array_element _lowestgrounded PlayerObject))))))

(fn LowestGrounded
  (params (BA :type Array%20of%20BA%20Object%20References))
  (for _array_element BA
    (if (or (< (+ (Variables|BA_C|GetGrounded _array_element) 1) (LocalVariables|Get_LowestGrounded)) (< (LocalVariables|Get_LowestGrounded) 0))
      (LocalVariables|Set_LowestGrounded (+ (Variables|BA_C|GetGrounded _array_element) 1))))
  (return (LocalVariables|Get_LowestGrounded)))

(fn OutlineMode
  (params (OutlineMode :type Boolean))
  (bind _returnvalue (Actor|GetComponentsByClass "/Script/Engine.StaticMeshComponent"))
  (if OutlineMode
    (for _array_element _returnvalue
      (Rendering|Material|SetMaterial _array_element 0 "/Game/GlobalMaterials/M_BuildingSelectOutline.M_BuildingSelectOutline"))
    (else
      (for (_array_element_2 _array_index) _returnvalue
        (Rendering|Material|SetMaterial _array_element_2 0 (Utilities|Array|Get(acopy) (Variables|Default|GetBuildingMaterials) _array_index))))))

(fn GetBuildingActor
  (return self))