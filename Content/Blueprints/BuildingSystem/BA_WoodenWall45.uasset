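; BA_WoodenWall45 is a placeable 45-degree wooden wall piece for the building system.
; The construction script sets the mesh variant from MBIndex, which also selects the offsets and roll of the placement trace.
; CheckPlacing runs a thin box trace on the Visibility channel, tilted 45 degrees either way and aligned to actor rotation, and blocks placement on a hit.
; It never reports ZeroGround, and GetBuildingActor returns the actor itself.
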(fn ConstructionScript
  (Components|StaticMesh|SetStaticMesh (Variables|Default|GetStaticMesh) (Utilities|Array|Get(acopy) (Variables|Default|GetMB_StaticMesh) (Variables|Default|GetMB_Index))))

(fn CheckPlacing
  (bind _returnvalue (Transformation|GetActorRotation))
  (bind _location (CallFunction|AddOffsettoActor "0.000000,115.000000,40.000000"))
  (bind _location_2 (CallFunction|AddOffsettoActor "0.000000,-40.000000,-115.000000"))
  (bind _mb_index (Variables|Default|GetMB_Index))
  (bind _returnvalue_2 (Collision|BoxTraceByChannel (Utilities|Select :Index _mb_index :Option%200 _location :Option%201 (CallFunction|VectorSignInvert _location false true false)) (Utilities|Select :Index _mb_index :Option%200 _location_2 :Option%201 (CallFunction|VectorSignInvert _location_2 false true false)) "8.000000,40.000000,1.000000" (Math|Rotator|MakeRotator (Utilities|Select :Index (Variables|Default|GetMB_Index) :Option%200 45.0 :Option%201 -45.0) (.pitch _returnvalue) (.yaw _returnvalue)) "TraceTypeQuery1" false 0 "None" true "(R=1.000000,G=0.000000,B=0.000000,A=1.000000)" "(R=0.000000,G=1.000000,B=0.000000,A=1.000000)" 2.0))
  (if _returnvalue_2
    (return false 0 false)
    (else
      (return true 0 false))))

(fn GetBuildingActor
  (return self))