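; BP_Building is the base actor for placeable building pieces, with preview, outline and collision modes plus stub placement checks.
; Supports/Depends links form a structural graph where Grounded tracks steps from ground, propagating on build or destroy and tinting previews.
; ServerDestroy refunds required items, recursively removes pieces left unsupported or beyond GroundedMax, and multicasts destroy effects.
; Corner line traces validate free placement when all four hit Building-tagged or all Island-tagged actors.
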(event Custom|Multicast_SpawnEffects
  (Niagara|SpawnSystemAttached "/Game/Particles/NS_BuildWood.NS_BuildWood" (Actor|GetComponentbyClass "/Script/Engine.StaticMeshComponent") "None" "0, 0, 0" "0, 0, 0" "KeepRelativeOffset" true)
  (Audio|SpawnSoundatLocation "/Game/Audio/SFX/BuildWood.BuildWood" (Transformation|GetActorLocation) "0, 0, 0" (Math|Random|RandomFloatinRange 0.8 1.2) (Math|Random|RandomFloatinRange 0.9 1.1) 0.0 "/Game/Audio/NormalAttenuation.NormalAttenuation" 0))

(event Custom|Multicast_DestroyEffects
  (Audio|SpawnSoundatLocation "/Game/Audio/SFX/DestroyWood.DestroyWood" (Transformation|GetActorLocation) "0, 0, 0" 0.5 (Math|Random|RandomFloatinRange 1.5 1.8) 0.0 "/Game/Audio/NormalAttenuation.NormalAttenuation" 0))

(fn ConstructionScript)

(fn PreviewMode
  (params (PreviewMode :type Boolean))
  (bind _returnvalue (Actor|GetComponentsByClass "/Script/Engine.StaticMeshComponent"))
  (if PreviewMode
    (for _array_element _returnvalue
      (Rendering|Material|SetMaterial _array_element 0 "/Game/MaterialsGlobal/M_BuildingPreview.M_BuildingPreview"))
    (else
      (for (_array_element_2 _array_index) _returnvalue
        (Rendering|Material|SetMaterial _array_element_2 0 (Utilities|Array|Get(acopy) (Variables|Default|GetAllMaterials) _array_index))))))

(fn CollisionMode
  (params (CollisionMode :type ECollisionEnabled%20Enum :default "NoCollision"))
  (bind _returnvalue (Utilities|Select :Index CollisionMode :NoCollision false :QueryOnly false :PhysicsOnly true :QueryAndPhysics true :ProbeOnly false :QueryAndProbe false))
  (Utilities|FlowControl|Sequence
    (:then_0
      (Collision|SetActorEnableCollision _returnvalue))
    (:then_1
      (for _array_element (Actor|GetAllChildActors false)
        (Collision|SetActorEnableCollision _array_element _returnvalue)))))

(fn OutlineMode
  (params (OutlineMode :type Boolean))
  (bind _returnvalue (Actor|GetComponentsByClass "/Script/Engine.StaticMeshComponent"))
  (if OutlineMode
    (for _array_element _returnvalue
      (Rendering|Material|SetMaterial _array_element 0 "/Game/MaterialsGlobal/M_BuildingSelectOutline.M_BuildingSelectOutline"))
    (else
      (for (_array_element_2 _array_index) _returnvalue
        (Rendering|Material|SetMaterial _array_element_2 0 (Utilities|Array|Get(acopy) (Variables|Default|GetAllMaterials) _array_index))))))

(fn SetPreviewColor
  (params (ColorPreview :type E_BuildingPartPreviewColor%20Enum :default "NewEnumerator0"))
  (bind _returnvalue (Math|Vector|MakeVector 0.1 0.1 1.0))
  (bind _returnvalue_2 (Actor|GetComponentsByClass "/Script/Engine.StaticMeshComponent"))
  (bind _grounded (Variables|Default|GetGrounded))
  (bind _groundedmax (Variables|Default|GetGroundedMax))
  (bind _returnvalue_3 (Math|Conversions|ToFloat(Byte) _groundedmax))
  (bind _returnvalue_4 (Math|Conversions|ToFloat(Byte) _grounded))
  (bind _returnvalue_5 (Math|Float|MapRangeClamped _returnvalue_4 0.0 _returnvalue_3 1.0 0.25))
  (bind _returnvalue_6 (Math|Float|MapRangeClamped _returnvalue_4 0.0 _returnvalue_3 0.0 0.85))
  (switch Utilities|FlowControl|Switch|SwitchonE_BuildingPartPreviewColor ColorPreview
    (:NewEnumerator0
      (for _array_element _returnvalue_2
        (Rendering|Material|SetVectorParameterValueonMaterials _array_element "BuildingPreviewColor" "1.000000, 0, 0")))
    (:NewEnumerator1
      (for _array_element_2 _returnvalue_2
        (Rendering|Material|SetVectorParameterValueonMaterials _array_element_2 "BuildingPreviewColor" _returnvalue)))
    (:NewEnumerator2
      (for _array_element_3 _returnvalue_2
        (Rendering|Material|SetVectorParameterValueonMaterials _array_element_3 "BuildingPreviewColor" (Math|Vector|MakeVector _returnvalue_6 _returnvalue_5 0.0))))
    (:NewEnumerator3
      (for _array_element_4 _returnvalue_2
        (Rendering|Material|SetVectorParameterValueonMaterials _array_element_4 "BuildingPreviewColor" (select (> _grounded 0) (Math|Vector|MakeVector _returnvalue_6 _returnvalue_5 0.0) _returnvalue))))))

(fn CheckPlacing
  (return false 0 false))

(fn UpdateGroundedonBuild
  (params (NewGrounded :type Byte))
  (Variables|Default|SetGrounded NewGrounded)
  (for _array_element (Variables|Default|GetSupports)
    (if (not (<= (Variables|/Script/SkyCraft.Building|GetGrounded _array_element) (+ 1 (Variables|Default|GetGrounded))))
      (bind _asbp_building (Utilities|Casting|CastToBP_Building _array_element))
      (CallFunction|UpdateGroundedonBuild _asbp_building (+ 1 (Variables|Default|GetGrounded))))))

(fn UpdateGroundedonDestroy
  (params (NewGrounded :type Byte) (CauserInventory :type Inventory%20Object%20Reference))
  (bind _output_get (Variables|Default|SetGrounded NewGrounded))
  (if (> _output_get (Variables|Default|GetGroundedMax))
    (CallFunction|ServerDestroy CauserInventory)
    (else
      (for _array_element (Variables|Default|GetSupports)
        (Utilities|IsValid _array_element
          (:Is%20Valid
            (bind _asbp_building (Utilities|Casting|CastToBP_Building _array_element))
            (bind _lowestgrounded (CallFunction|LowestGrounded _asbp_building))
            (if (!= _lowestgrounded (Variables|/Script/SkyCraft.Building|GetGrounded _array_element))
              (CallFunction|UpdateGroundedonDestroy _asbp_building _lowestgrounded CauserInventory))))))))

(fn LowestGrounded
  (for _array_element (Variables|Default|GetDepends)
    (if (or (< (+ (Variables|/Script/SkyCraft.Building|GetGrounded _array_element) 1) (LocalVariables|Get_LowestGrounded)) (< (LocalVariables|Get_LowestGrounded) 1))
      (LocalVariables|Set_LowestGrounded (+ (Variables|/Script/SkyCraft.Building|GetGrounded _array_element) 1))))
  (return (LocalVariables|Get_LowestGrounded)))

(fn AddOffsettoActor
  (params (Offset :type Vector))
  (bind _defaultsceneroot (Variables|Default|GetDefaultSceneRoot))
  (return (+ (Transformation|GetActorLocation) (* (Math|Vector|GetForwardVector _defaultsceneroot) (.x Offset)) (* (Math|Vector|GetRightVector _defaultsceneroot) (.y Offset)) (* (Math|Vector|GetUpVector _defaultsceneroot) (.z Offset)))))

(fn RecursiveDestroy
  (params (CauserInventory :type Inventory%20Object%20Reference) (inFlaggedDestroy :type Array%20of%20Building%20Object%20References))
  (Utilities|Array|Add inFlaggedDestroy self)
  (for _array_element (Variables|Default|GetSupports)
    (Utilities|IsValid _array_element
      (:Is%20Valid
        (Utilities|Array|Clear (LocalVariables|Get_checkedDepends))
        (if (not (Utilities|Array|ContainsItem inFlaggedDestroy _array_element))
          (Utilities|Array|RemoveItem (Variables|/Script/SkyCraft.Building|GetDepends _array_element) self)
          (bind _asbp_building (Utilities|Casting|CastToBP_Building _array_element)
            (:then
              _)
            (:CastFailed
              _))
          (bind _supported (CallFunction|IsSupported _asbp_building (LocalVariables|Get_checkedDepends)))
          (if (not _supported)
            (CallFunction|RecursiveDestroy _asbp_building CauserInventory inFlaggedDestroy))))))
  (for _array_element_2 (Variables|/Script/SkyCraft.DA_Building|GetRequiredItems (Variables|Default|GetDA_Building))
    (Default|Add CauserInventory _array_element_2))
  (Actor|DestroyActor))

(fn ServerDestroy
  (params (CauserInventory :type Inventory%20Object%20Reference))
  (bind _da_building (Variables|Default|GetDA_Building))
  (Utilities|Array|Add (LocalVariables|Get_flaggedDestroy) self)
  (Utilities|IsValid _da_building
    (:Is%20Valid
      (for _array_element (Variables|/Script/SkyCraft.DA_Building|GetRequiredItems _da_building)
        (Default|Add CauserInventory _array_element)))
    (:Is%20Not%20Valid
      (CallFunction|AdianPrintError (Utilities|String|Append "BUILDING DATA ASSET IS NOT VALID: " (Utilities|GetDisplayName self)))))
  (Utilities|FlowControl|Sequence
    (:then_0
      (for _array_element_2 (Variables|Default|GetSupports)
        (Utilities|IsValid _array_element_2
          (:Is%20Valid
            (Utilities|Array|Clear (LocalVariables|Get_checkedDepends))
            (Utilities|Array|Add (LocalVariables|Get_checkedDepends) self)
            (Utilities|Array|RemoveItem (Variables|/Script/SkyCraft.Building|GetSupports _array_element_2) self)
            (Utilities|Array|RemoveItem (Variables|/Script/SkyCraft.Building|GetDepends _array_element_2) self)
            (bind _asbp_building (Utilities|Casting|CastToBP_Building _array_element_2)
              (:then
                _)
              (:CastFailed
                _))
            (bind _supported (CallFunction|IsSupported _asbp_building (LocalVariables|Get_checkedDepends)))
            (if _supported
              (bind _lowestgrounded (CallFunction|LowestGrounded _asbp_building))
              (CallFunction|UpdateGroundedonDestroy _asbp_building _lowestgrounded CauserInventory)
              (else
                (CallFunction|RecursiveDestroy _asbp_building CauserInventory (LocalVariables|Get_flaggedDestroy))))))))
    (:then_1
      (Utilities|FlowControl|Sequence
        (:then_0
          (for _array_element_3 (Variables|Default|GetDepends)
            (Utilities|IsValid _array_element_3
              (:Is%20Valid
                (Utilities|Array|RemoveItem (Variables|/Script/SkyCraft.Building|GetSupports _array_element_3) self)))))
        (:then_1
          (CallFunction|MulticastDestroyEffects)
          (Actor|DestroyActor))))))

(fn IsSupported
  (params (CheckedDepends :type Array%20of%20Building%20Object%20References))
  (if (<= (Variables|Default|GetGrounded) 0)
    (return true)
    (else
      (Utilities|Array|Add CheckedDepends self)
      (for _array_element (Variables|Default|GetDepends)
        (Utilities|IsValid _array_element
          (:Is%20Valid
            (if (not (Utilities|Array|ContainsItem CheckedDepends _array_element))
              (if (<= (Variables|/Script/SkyCraft.Building|GetGrounded _array_element) 0)
                (return true)
                (else
                  (bind _asbp_building (Utilities|Casting|CastToBP_Building _array_element))
                  (bind _supported (CallFunction|IsSupported _asbp_building CheckedDepends))
                  (if _supported
                    (return true))))))))
      (return false))))

(fn CornersLinetraces
  (params (Dimensions :type Vector%202D%20Structure) (Debug :type Boolean))
  (bind _returnvalue (Transformation|GetActorLocation))
  (bind _returnvalue_2 (Transformation|GetActorRotation))
  (bind _returnvalue_3 (/ (.x Dimensions) 2.0))
  (bind _returnvalue_4 (/ (.y Dimensions) 2.0))
  (bind __uniquefloors (LocalVariables|Get_UniqueFloors))
  (bind _returnvalue_5 (Math|Vector|GetRightVector _returnvalue_2))
  (bind _returnvalue_6 (Math|Vector|GetForwardVector _returnvalue_2))
  (bind _returnvalue_7 (+ _returnvalue "0,0,5.000000"))
  (bind _returnvalue_8 (select Debug "ForOneFrame" "None"))
  (bind _returnvalue_9 (* _returnvalue_4 _returnvalue_5 -1.0))
  (bind _returnvalue_10 (* _returnvalue_3 _returnvalue_6 -1.0))
  (bind _returnvalue_11 (* _returnvalue_3 _returnvalue_6))
  (bind _returnvalue_12 (* _returnvalue_4 _returnvalue_5))
  (bind _returnvalue_13 (+ _returnvalue_11 _returnvalue_12 _returnvalue_7))
  (bind _returnvalue_14 (+ _returnvalue_11 _returnvalue_9 _returnvalue_7))
  (bind _returnvalue_15 (+ _returnvalue_10 _returnvalue_9 _returnvalue_7))
  (bind _returnvalue_16 (+ _returnvalue_10 _returnvalue_12 _returnvalue_7))
  (bind _outhit (Collision|LineTraceByChannel _returnvalue_13 (+ _returnvalue_13 "0,0,-10.000000") "TraceTypeQuery1" false 0 _returnvalue_8))
  (bind _outhit_2 (Collision|LineTraceByChannel _returnvalue_14 (+ _returnvalue_14 "0,0,-10.000000") "TraceTypeQuery1" false 0 _returnvalue_8))
  (bind _outhit_3 (Collision|LineTraceByChannel _returnvalue_15 (+ _returnvalue_15 "0.000000,0.000000,-10.000000") "TraceTypeQuery1" false 0 _returnvalue_8))
  (bind _outhit_4 (Collision|LineTraceByChannel _returnvalue_16 (+ _returnvalue_16 "0.000000,0.000000,-10.000000") "TraceTypeQuery1" false 0 _returnvalue_8))
  (Utilities|Array|AddUnique __uniquefloors (.HitActor (Collision|BreakHitResult _outhit_2)))
  (Utilities|Array|AddUnique __uniquefloors (.HitActor (Collision|BreakHitResult _outhit)))
  (Utilities|Array|AddUnique __uniquefloors (.HitActor (Collision|BreakHitResult _outhit_3)))
  (Utilities|Array|AddUnique __uniquefloors (.HitActor (Collision|BreakHitResult _outhit_4)))
  (if (Math|Boolean|ANDBoolean (CallFunction|ActorHasSkyTag (.HitActor (Collision|BreakHitResult _outhit_2)) "/Game/DataAssets/SkyTag/Building.Building") (CallFunction|ActorHasSkyTag (.HitActor (Collision|BreakHitResult _outhit)) "/Game/DataAssets/SkyTag/Building.Building") (CallFunction|ActorHasSkyTag (.HitActor (Collision|BreakHitResult _outhit_3)) "/Game/DataAssets/SkyTag/Building.Building") (CallFunction|ActorHasSkyTag (.HitActor (Collision|BreakHitResult _outhit_4)) "/Game/DataAssets/SkyTag/Building.Building"))
    (return true (LocalVariables|Get_UniqueFloors))
    (elif (Math|Boolean|ANDBoolean (CallFunction|ActorHasSkyTag (.HitActor (Collision|BreakHitResult _outhit_2)) "/Game/DataAssets/SkyTag/Island.Island") (CallFunction|ActorHasSkyTag (.HitActor (Collision|BreakHitResult _outhit)) "/Game/DataAssets/SkyTag/Island.Island") (CallFunction|ActorHasSkyTag (.HitActor (Collision|BreakHitResult _outhit_3)) "/Game/DataAssets/SkyTag/Island.Island") (CallFunction|ActorHasSkyTag (.HitActor (Collision|BreakHitResult _outhit_4)) "/Game/DataAssets/SkyTag/Island.Island"))
      (return true (LocalVariables|Get_UniqueFloors))
      (else
        (return false 0)))))

(fn FreeBuildingLinetraces
  (params (Debug :type Boolean))
  (bind (_valid _uniquefloors) (CallFunction|CornersLinetraces "(X=0.000000,Y=0.000000)" Debug))
  (return _valid _uniquefloors))

(fn CheckFreeBuildingPlacing
  (return false 0))

(fn GetSkyTags
  (return (Utilities|Struct|MakeGetSkyTagsOut (Variables|/Script/SkyCraft.SkyTags|GetDA_SkyTags (Variables|Default|GetSkyTags)))))