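; Placeable wooden storage chest for the building system, with an inventory that is saved and loaded through its building parameters.
; Free placement requires valid floor traces across its footprint and a clear box trace, then attaches to the first floor found.
; Interacting opens a chest widget on the client, while the server tracks interacting players and multicasts their count.
; That count drives a timeline that swings the lid open, or closed once nobody remains.
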(event Custom|Multicast_OpenCloseChest
  (params (InteractedPlayers :type Integer))
  (if (> InteractedPlayers 0)
    (if (not (Variables|Default|GetChestOpened))
      (CallFunction|ToggleChest true))
    (elif (Variables|Default|GetChestOpened)
      (CallFunction|ToggleChest false))))

(event Custom|ToggleChest
  (params (Open :type Boolean))
  (bind _output_get (Variables|Default|SetChestOpened Open))
  (if _output_get
    (bind _newtrack_0 (Timeline|Timeline_OpenChest PlayFromStart)
      (:Update
        (Transformation|SetRelativeRotation (Variables|Default|GetTop) (Math|Rotator|MakeRotator _newtrack_0 0.0 0.0) false false)))
    (else
      (Timeline|Timeline_OpenChest ReverseFromEnd))))

(event EventTick
  (params (DeltaSeconds :type Float%20%28single-precision%29)))

(fn ConstructionScript)

(fn SaveBuildingParameters
  (return (Utilities|Struct|MakeBuildingParameters 0 0 (Utilities|Array|MakeArray (Utilities|Struct|MakeArrayInventorySlots (Variables|/Script/SkyCraft.Inventory|GetSlots (Variables|Default|GetInventory)))))))

(fn LoadBuildingParameters
  (params (BuildingParameters :type Building%20Parameters%20Structure))
  (Variables|/Script/SkyCraft.Inventory|SetSlots (Variables|Default|GetInventory) (Utilities|Struct|BreakArrayInventorySlots (Utilities|Array|Get(acopy) (.ArrayInventorySlots (Utilities|Struct|BreakBuildingParameters BuildingParameters)))))
  (return true))

(fn CheckFreeBuildingPlacing
  (bind _returnvalue (Transformation|GetActorLocation))
  (bind (_valid _uniquefloors) (CallFunction|FreeBuildingLinetraces false))
  (if _valid
    (bind _returnvalue_2 (Collision|BoxTraceByChannel (+ _returnvalue "0,0,6.000000") (+ _returnvalue "0,0.000000,60.000000") "40.000000,40.000000,1.000000" (Transformation|GetActorRotation) "TraceTypeQuery1" false 0 "None" true "(R=1.000000,G=0.000000,B=0.000000,A=1.000000)" "(R=0.000000,G=1.000000,B=0.000000,A=1.000000)" 2.0))
    (if (not _returnvalue_2)
      (return true (Utilities|Array|Get(acopy) _uniquefloors))
      (else
        (return false 0)))
    (else
      (return false 0))))

(fn CornersLinetraces
  (params (Dimensions :type Vector%202D%20Structure) (Debug :type Boolean))
  (bind (_valid _uniquefloors) (|CallParentFunction "(X=70.000000,Y=70.000000)" Debug))
  (return _valid _uniquefloors))

(fn ClientInteractBP
  (params (InteractKey :type EInteractKey%20Enum :default "Interact1") (Pawn :type Pawn%20Object%20Reference) (BP_PSS :type BP%20PSS%20Object%20Reference))
  (switch Utilities|FlowControl|Switch|SwitchonEInteractKey InteractKey
    (:Interact1
      (Utilities|IsValid (Variables|Default|GetCWS_Chest)
        (:Is%20Valid
          _)
        (:Is%20Not%20Valid
          (bind _returnvalue (UserInterface|CreateWidget "/Game/Widgets/CWS/CWS_Chest.CWS_Chest_C" 0 self))
          (Variables|Default|SetCWS_Chest _returnvalue)))
      (UserInterface|Viewport|AddtoViewport (Variables|Default|GetCWS_Chest) 10)
      (Default|AddCWS BP_PSS (Variables|Default|GetCWS_Chest) true true "NewEnumerator2")
      (Default|SetMousetoCenter BP_PSS)
      (return true))))

(fn ClientInterruptBP
  (params (InterruptedBy :type EInterruptedBy%20Enum :default "Player") (InteractKey :type EInteractKey%20Enum :default "Interact1") (Pawn :type Pawn%20Object%20Reference) (BP_PSS :type BP%20PSS%20Object%20Reference))
  (return false))

(fn ServerInteractBP
  (params (InteractKey :type EInteractKey%20Enum :default "Interact1") (Pawn :type Pawn%20Object%20Reference) (BP_PSS :type BP%20PSS%20Object%20Reference))
  (bind _interactplayers (Variables|Default|GetInteractPlayers))
  (switch Utilities|FlowControl|Switch|SwitchonEInteractKey InteractKey
    (:Interact1
      (Utilities|Array|Add _interactplayers Pawn)
      (CallFunction|MulticastOpenCloseChest (Utilities|Array|Length _interactplayers))
      (return true))))

(fn ServerInterruptBP
  (params (InterruptedBy :type EInterruptedBy%20Enum :default "Player") (InteractKey :type EInteractKey%20Enum :default "Interact1") (Pawn :type Pawn%20Object%20Reference) (BP_PSS :type BP%20PSS%20Object%20Reference))
  (bind _interactplayers (Variables|Default|GetInteractPlayers))
  (Utilities|Array|RemoveItem _interactplayers Pawn)
  (CallFunction|MulticastOpenCloseChest (Utilities|Array|Length _interactplayers))
  (return true))