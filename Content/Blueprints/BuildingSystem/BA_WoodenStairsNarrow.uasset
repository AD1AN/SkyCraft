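; Narrow wooden stairs piece for the building system, with its own placement check run from the construction script.
; CheckPlacing sweeps a pitched box trace beneath the stairs, placed by actor-relative offsets and the actor's rotation.
; A hit allows placement and flags ZeroGround only if the actor is tagged Island; no hit allows placement without ground.
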(fn ConstructionScript
  (CallFunction|CheckPlacing))

(fn CheckPlacing
  (bind _returnvalue (Transformation|GetActorRotation))
  (bind (_outhit _returnvalue_2) (Collision|BoxTraceByChannel (CallFunction|AddOffsettoActor "125.000000,0.000000,-15.000000") (CallFunction|AddOffsettoActor "-90.000000,0.000000,-120.000000") "5.000000,40.000000,10.000000" (Math|Rotator|MakeRotator (.roll _returnvalue) 26.5 (.yaw _returnvalue)) "TraceTypeQuery1" false 0 "None" true "(R=1.000000,G=0.000000,B=0.000000,A=1.000000)" "(R=0.000000,G=1.000000,B=0.000000,A=1.000000)" 2.0))
  (if _returnvalue_2
    (return (Actor|ActorHasTag (.HitActor (Collision|BreakHitResult _outhit)) "Island") 0 (Actor|ActorHasTag (.HitActor (Collision|BreakHitResult _outhit)) "Island"))
    (else
      (return true 0 false))))