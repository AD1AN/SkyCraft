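; Placeable wooden door for the building system that players tap to swing open or closed in multiplayer.
; A server tap interaction, ignored mid-animation, multicasts a timeline yaw swing, which then calls a server event to flip Opened.
; Opened's RepNotify snaps the mesh to its resting yaw only when no animation is flagged, syncing clients that missed the swing.
; Placement checking uses a box trace to block obstructed spots and recolor the preview.
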(event Custom|Multicast_ToggleDoor
  (Variables|Default|SetAnimated true)
  (if (Variables|Default|GetOpened)
    (bind _newtrack_0 (Timeline|DoorTimeline ReverseFromEnd)
      (:Update
        (Transformation|SetRelativeRotation (Variables|Default|GetStaticMesh) (Math|Rotator|MakeRotator 0.0 0.0 (Math|Float|Lerp -9e+01 -2e+02 _newtrack_0)) false false))
      (:Finished
        (CallFunction|ServerToggleDoor)
        (Variables|Default|SetAnimated false)))
    (else
      (Timeline|DoorTimeline PlayFromStart))))

(event Custom|Server_ToggleDoor
  (Variables|Default|SetOpened (not (Variables|Default|GetOpened))))

(fn ConstructionScript)

(fn CheckPlacing
  (bind _returnvalue (Collision|BoxTraceByChannel (CallFunction|AddOffsettoActor "0,-66.599998,55.000000") (CallFunction|AddOffsettoActor "0.000000,-66.599998,-125.000000") "5.000000,60.000000,5.000000" (Transformation|GetActorRotation) "TraceTypeQuery1" false 0 "None" true "(R=1.000000,G=0.000000,B=0.000000,A=1.000000)" "(R=0.000000,G=1.000000,B=0.000000,A=1.000000)" 2.0))
  (if _returnvalue
    (CallFunction|SetPreviewColor "NewEnumerator0")
    (return false 0 false)
    (else
      (CallFunction|SetPreviewColor "NewEnumerator2")
      (return true 0 false))))

(fn OnRepOpened
  (if (Variables|Default|GetAnimated)
    (Variables|Default|SetAnimated false)
    (else
      (Transformation|SetRelativeRotation (Variables|Default|GetStaticMesh) (Math|Rotator|MakeRotator 0.0 0.0 (Math|Float|SelectFloat -2e+02 -9e+01 (Variables|Default|GetOpened))) false false))))

(fn ClientInterrupt
  (params (InterruptedBy :type E_InterruptedBy%20Enum :default "NewEnumerator0") (InteractKey :type E_InteractKey%20Enum :default "NewEnumerator0") (InteractedPawn :type Pawn%20Object%20Reference) (InteractedPC_Sky :type PC%20Sky%20Object%20Reference))
  (return false))

(fn ClientTapInteract
  (params (InteractedKey :type E_InteractKey%20Enum :default "NewEnumerator0") (InteractedPawn :type Pawn%20Object%20Reference) (InteractedPC_Sky :type PC%20Sky%20Object%20Reference) (InteractedWith :type IC%20Class%20Reference))
  (return false))

(fn GetInteractLocation
  (return "0, 0, 0"))

(fn GetInteractSystem
  (return 0))

(fn ServerInterrupt
  (params (InterruptedBy :type E_InterruptedBy%20Enum :default "NewEnumerator0") (InteractKey :type E_InteractKey%20Enum :default "NewEnumerator0") (InteractedPawn :type Pawn%20Object%20Reference) (InteractedPC_Sky :type PC%20Sky%20Object%20Reference))
  (return false))

(fn ServerTapInteract
  (params (InteractedKey :type E_InteractKey%20Enum :default "NewEnumerator0") (InteractedPawn :type Pawn%20Object%20Reference) (InteractedPC_Sky :type PC%20Sky%20Object%20Reference) (InteractedWith :type IC%20Class%20Reference))
  (if (not (Variables|Default|GetAnimated))
    (CallFunction|MulticastToggleDoor)
    (return true)))