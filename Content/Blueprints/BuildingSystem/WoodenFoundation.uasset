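; Wooden foundation piece for the building system, which overrides the placement check for setting it on island ground.
; CheckPlacing rejects the spot and sets the preview color if a box trace at the actor's location hits anything.
; Otherwise, four downward corner box traces must all hit Island-tagged actors.
; Success reports zero ground and returns one hit actor as the attachment target; an alternative foundation-on-foundation condition is left unused.
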(fn ConstructionScript
  (|CallParentFunction))

(fn CheckPlacing
  (bind _returnvalue (Transformation|GetActorLocation))
  (LocalVariables|Set_ARot (Transformation|GetActorRotation))
  (bind _returnvalue_2 (Collision|BoxTraceByChannel _returnvalue _returnvalue "140.000000,140.000000,10.000000" (LocalVariables|Get_ARot) "TraceTypeQuery1" false 0 "None" true "(R=1.000000,G=0.000000,B=0.000000,A=1.000000)" "(R=0.000000,G=1.000000,B=0.000000,A=1.000000)" 2.0))
  (if _returnvalue_2
    (CallFunction|SetPreviewColor "NewEnumerator0")
    (return false 0 false)
    (else
      (bind (_outhit _returnvalue_3) (Collision|BoxTraceByChannel (CallFunction|AddOffsettoActor "125.000000,125.000000,-15.000000") (CallFunction|AddOffsettoActor "125.000000,125.000000,-280.000000") "15.000000,15.000000,10.000000" (LocalVariables|Get_ARot) "TraceTypeQuery1" false 0 "None" true "(R=1.000000,G=0.000000,B=0.000000,A=1.000000)" "(R=0.000000,G=1.000000,B=0.000000,A=1.000000)" 2.0))
      (bind (_outhit_2 _returnvalue_4) (Collision|BoxTraceByChannel (CallFunction|AddOffsettoActor "-125.000000,-125.000000,-15.000000") (CallFunction|AddOffsettoActor "-125.000000,-125.000000,-280.000000") "15.000000,15.000000,10.000000" (LocalVariables|Get_ARot) "TraceTypeQuery1" false 0 "None" true "(R=1.000000,G=0.000000,B=0.000000,A=1.000000)" "(R=0.000000,G=1.000000,B=0.000000,A=1.000000)" 2.0))
      (bind (_outhit_3 _returnvalue_5) (Collision|BoxTraceByChannel (CallFunction|AddOffsettoActor "125.000000,-125.000000,-15.000000") (CallFunction|AddOffsettoActor "125.000000,-125.000000,-280.000000") "15.000000,15.000000,10.000000" (LocalVariables|Get_ARot) "TraceTypeQuery1" false 0 "None" true "(R=1.000000,G=0.000000,B=0.000000,A=1.000000)" "(R=0.000000,G=1.000000,B=0.000000,A=1.000000)" 2.0))
      (bind (_outhit_4 _returnvalue_6) (Collision|BoxTraceByChannel (CallFunction|AddOffsettoActor "-125.000000,125.000000,-15.000000") (CallFunction|AddOffsettoActor "-125.000000,125.000000,-280.000000") "15.000000,15.000000,10.000000" (LocalVariables|Get_ARot) "TraceTypeQuery1" false 0 "None" true "(R=1.000000,G=0.000000,B=0.000000,A=1.000000)" "(R=0.000000,G=1.000000,B=0.000000,A=1.000000)" 2.0))
      (if (Math|Boolean|ANDBoolean _returnvalue_6 _returnvalue_5 _returnvalue_4 _returnvalue_3)
        (if (Math|Boolean|ANDBoolean (CallFunction|ActorHasSkyTag (.HitActor (Collision|BreakHitResult _outhit)) "/Game/DataAssets/SkyTag/Island.Island") (CallFunction|ActorHasSkyTag (.HitActor (Collision|BreakHitResult _outhit_2)) "/Game/DataAssets/SkyTag/Island.Island") (CallFunction|ActorHasSkyTag (.HitActor (Collision|BreakHitResult _outhit_3)) "/Game/DataAssets/SkyTag/Island.Island") (CallFunction|ActorHasSkyTag (.HitActor (Collision|BreakHitResult _outhit_4)) "/Game/DataAssets/SkyTag/Island.Island"))
          (return true (.HitActor (Collision|BreakHitResult _outhit_4)) true)
          (else
            _)))
      (return false 0 false))))