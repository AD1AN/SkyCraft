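; Workbench is a placeable structure in the building system that opens a crafting-station style UI (CWS_Workbench) when used.
; Free placement requires valid floor linetraces and a clear box trace above the actor, then attaches to the first floor found.
; It overrides the parent's corner traces with its own fixed footprint.
; Interact 1 creates the widget client-side, registers it with BPPSS and centers the mouse; server interaction and interrupt handlers just return false.
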(fn ConstructionScript)

(fn CheckFreeBuildingPlacing
  (bind _returnvalue (Transformation|GetActorLocation))
  (bind (_valid _uniquefloors) (CallFunction|FreeBuildingLinetraces false))
  (if _valid
    (bind _returnvalue_2 (Collision|BoxTraceByChannel (+ _returnvalue "0,0,6.000000") (+ _returnvalue "0.000000,0.000000,120.000000") "50.000000,70.000000,1.000000" (Transformation|GetActorRotation) "TraceTypeQuery1" false 0 "None" true "(R=1.000000,G=0.000000,B=0.000000,A=1.000000)" "(R=0.000000,G=1.000000,B=0.000000,A=1.000000)" 2.0))
    (if (not _returnvalue_2)
      (return true (Utilities|Array|Get(acopy) _uniquefloors))
      (else
        (return false 0)))
    (else
      (return false 0))))

(fn CornersLinetraces
  (params (Dimensions :type Vector%202D%20Structure) (Debug :type Boolean))
  (bind (_valid _uniquefloors) (|CallParentFunction "(X=70.000000,Y=140.000000)" Debug))
  (return _valid _uniquefloors))

(fn ClientInteractBP
  (params (InteractKey :type EInteractKey%20Enum :default "Interact1") (Pawn :type Pawn%20Object%20Reference) (BP_PSS :type BP%20PSS%20Object%20Reference))
  (switch Utilities|FlowControl|Switch|SwitchonEInteractKey InteractKey
    (:Interact1
      (bind _returnvalue (UserInterface|CreateWidget "/Game/Widgets/CWS/CWS_Workbench.CWS_Workbench_C"))
      (UserInterface|Viewport|AddtoViewport _returnvalue 25)
      (Default|AddCWS BP_PSS _returnvalue true true "NewEnumerator2")
      (Default|SetMousetoCenter BP_PSS)
      (return true))))

(fn ClientInterruptBP
  (params (InterruptedBy :type EInterruptedBy%20Enum :default "Player") (InteractKey :type EInteractKey%20Enum :default "Interact1") (Pawn :type Pawn%20Object%20Reference) (BP_PSS :type BP%20PSS%20Object%20Reference))
  (return false))

(fn ServerInteractBP
  (params (InteractKey :type EInteractKey%20Enum :default "Interact1") (Pawn :type Pawn%20Object%20Reference) (BP_PSS :type BP%20PSS%20Object%20Reference))
  (return false))

(fn ServerInterruptBP
  (params (InterruptedBy :type EInterruptedBy%20Enum :default "Player") (InteractKey :type EInteractKey%20Enum :default "Interact1") (Pawn :type Pawn%20Object%20Reference) (BP_PSS :type BP%20PSS%20Object%20Reference))
  (return false))