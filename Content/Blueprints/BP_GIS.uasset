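; Game Instance that loads local settings and manages multiplayer sessions for hosting, joining and invites.
; Hosting creates an advanced session from BPGSS options tagged with the world name, then opens SkyMain as a listen server, or restores the main menu on failure.
; Joins and accepted invites wait for a loading screen before joining, sharing one failure popup.
; Received invites spawn an invitation widget, replacing any existing one.
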(event Custom|HostGame
  (bind _w_loadingscreen (Variables|Default|GetW_LoadingScreen))
  (bind _bp_gss (Variables|Default|GetBP_GSS))
  (|AdvancedSession (Utilities|Array|MakeArray (Class|AdvancedSessionsLibrary|MakeLiteralSessionPropertyString "WorldName" (Variables|Default|GetLoadWorldName))) (Variables|Default|GetPC_MainMenu) 100 100 (Variables|/Script/SkyCraft.GSS|GetbUseLAN _bp_gss) (Variables|/Script/SkyCraft.GSS|GetbAllowInvites _bp_gss) false true (Variables|/Script/SkyCraft.GSS|GetbAllowJoinViaPresence _bp_gss) (Variables|/Script/SkyCraft.GSS|GetbAllowJoinViaPresenceFriendsOnly _bp_gss) false true (Variables|/Script/SkyCraft.GSS|GetbShouldAdvertise _bp_gss) false true
    (:OnSuccess
      (Game|OpenLevel(byObjectReference) "/Game/Levels/SkyMain.SkyMain" true "?listen")
      (Variables|Default|SetExitedMainMenu true))
    (:OnFailure
      (Utilities|IsValid _w_loadingscreen
        (:Is%20Valid
          (Widget|RemovefromParent _w_loadingscreen))
        (:Is%20Not%20Valid
          _))
      (Input|SetInputModeGameandUI (Variables|Default|GetPC_MainMenu) (Variables|Default|GetCurrent_W_MainMenu) "DoNotLock" false false)
      (Widget|SetVisibility (Variables|Default|GetCurrent_W_MainMenu) "Visible"))))

(event Custom|OnShowCompleted
  (Utilities|FlowControl|Delay 0.5)
  (|JoinSession (Variables|Default|GetPC_MainMenu) (stale Custom|OnlineJoinGame SessionResult)
    (:OnFailure
      (Widget|RemovefromParent (Variables|Default|GetW_LoadingScreen))
      (bind _returnvalue (UserInterface|CreateWidget "/Game/Widgets/W_JoinSessionFail.W_JoinSessionFail_C"))
      (Default|AddStackWidget (Variables|Default|GetPC_MainMenu) _returnvalue)
      (UserInterface|Viewport|AddtoViewport _returnvalue 100))))

(event Custom|OnShowCompleted_Accepted
  (Utilities|FlowControl|Delay 0.5)
  (|JoinSession (Variables|Default|GetPC_MainMenu) (stale EventOnSessionInviteAccepted SessionToJoin)
    (:OnFailure
      (Widget|RemovefromParent (Variables|Default|GetW_LoadingScreen))
      (bind _returnvalue (UserInterface|CreateWidget "/Game/Widgets/W_JoinSessionFail.W_JoinSessionFail_C"))
      (Default|AddStackWidget (Variables|Default|GetPC_MainMenu) _returnvalue)
      (UserInterface|Viewport|AddtoViewport _returnvalue 100))))

(event Custom|OnlineJoinGame
  (params (SessionResult :type Blueprint%20Session%20Result%20Structure%20%28by%20ref%29))
  (CallFunction|CreateLoadingScreen)
  (Default|ShowLoadingScreen (Variables|Default|GetW_LoadingScreen) (delegate Custom|OnShowCompleted) 4.0))

(event EventOnSessionInviteAccepted
  (params (LocalPlayerNum :type Integer) (PersonInvited :type BP%20Unique%20Net%20Id%20Structure) (SessionToJoin :type Blueprint%20Session%20Result%20Structure%20%28by%20ref%29))
  (CallFunction|CreateLoadingScreen)
  (Default|ShowLoadingScreen (Variables|Default|GetW_LoadingScreen) (delegate Custom|OnShowCompleted_Accepted) 4.0))

(event EventInit
  (bind _localsettings (CallFunction|LoadLocalSettings))
  (Variables|Default|SetLocalSettings _localsettings))

(event EventOnSessionInviteReceived
  (params (LocalPlayerNum :type Integer) (PersonInviting :type BP%20Unique%20Net%20Id%20Structure) (AppId :type String) (SessionToJoin :type Blueprint%20Session%20Result%20Structure%20%28by%20ref%29))
  (CallFunction|CreateInvitation PersonInviting SessionToJoin))

(fn CreateLoadingScreen
  (Utilities|IsValid (Variables|Default|GetW_LoadingScreen)
    (:Is%20Valid
      (Widget|RemovefromParent (Variables|Default|GetW_LoadingScreen)))
    (:Is%20Not%20Valid
      _))
  (bind _returnvalue (UserInterface|CreateWidget "/Game/Widgets/W_LoadingScreen.W_LoadingScreen_C" 0 0))
  (bind _output_get (Variables|Default|SetW_LoadingScreen _returnvalue))
  (UserInterface|Viewport|AddtoViewport _output_get 1000)
  (return))

(fn CreateInvitation
  (params (BPUniqueNetId :type BP%20Unique%20Net%20Id%20Structure) (SessionResult :type Blueprint%20Session%20Result%20Structure))
  (Utilities|IsValid (Variables|Default|GetW_Invitation)
    (:Is%20Valid
      (Widget|RemovefromParent (Variables|Default|GetW_Invitation)))
    (:Is%20Not%20Valid
      _))
  (bind _returnvalue (UserInterface|CreateWidget "/Game/Widgets/W_Invitation.W_Invitation_C" 0 BPUniqueNetId SessionResult))
  (bind _output_get (Variables|Default|SetW_Invitation _returnvalue))
  (UserInterface|Viewport|AddtoViewport _output_get 900))