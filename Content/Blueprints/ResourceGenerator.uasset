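; Resource generator component that procedurally scatters resource actors over its owning island actor.
; GenerateResources lays a jittered grid, sized and scaled by the island's scale ratio, and line-traces each cell for ground.
; Hits with matching collision tags and slopes under 35 degrees spawn attached resources with random yaw, size and mesh variety.
; Random streams are reseeded per point from the seed, generation count and point index for repeatable layouts.
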(fn SetupGenerator
  (params (AreaSize :type Float%20%28double-precision%29) (GeneratorSeed :type Integer) (ScaleRatio :type Float%20%28double-precision%29) (GroundAltitude :type Float%20%28double-precision%29) (LinetraceLength :type Float%20%28double-precision%29))
  (Variables|Default|SetAreaSize AreaSize)
  (Variables|Default|SetGeneratorSeed GeneratorSeed)
  (Variables|Default|SetScaleRatio ScaleRatio)
  (Variables|Default|SetGroundAltitude GroundAltitude)
  (Variables|Default|SetLinetraceLength LinetraceLength))

(fn GenerateResources
  (params (MaxSpawnPoints :type Integer) (DA_Resource :type DA%20Resource%20Object%20Reference) (ResourceSize :type S%20Int%20Min%20Max%20Structure) (SM_Variety :type S%20Int%20Min%20Max%20Structure))
  (bind _generations (Variables|Default|GetGenerations))
  (bind _generatorseed (Variables|Default|GetGeneratorSeed))
  (bind _scaleratio (Variables|Default|GetScaleRatio))
  (bind _areasize (Variables|Default|GetAreaSize))
  (bind _scaleratio_2 (Variables|Default|GetScaleRatio))
  (bind __spawnpointindex (LocalVariables|Get_SpawnPointIndex))
  (bind _returnvalue (Math|Float|Clamp(Float) _scaleratio 0.25 0.5))
  (bind _returnvalue_2 (+ _generatorseed _generations))
  (bind _returnvalue_3 (/ _areasize 2.0))
  (bind _returnvalue_4 (* _returnvalue _returnvalue_3))
  (Utilities|FlowControl|Sequence
    (:then_0
      (bind _output_get (LocalVariables|Set_SpawnPoints (Math|Float|Truncate (/ MaxSpawnPoints (- (- 3.0 _scaleratio_2) _scaleratio_2)))))
      (LocalVariables|Set_GridSize (Math|Float|Sqrt (Math|Conversions|ToFloat(Integer) _output_get)))
      (LocalVariables|Set_CellSize (/ (Variables|Default|GetAreaSize) (LocalVariables|Get_GridSize)))
      (LocalVariables|Set_MaxOffset (* 0.35 (LocalVariables|Get_CellSize)))
      (for _index (range 0 (- (Math|Float|Truncate (LocalVariables|Get_GridSize)) 1))
        (LocalVariables|Set_Row _index)
        (for _index_2 (range 0 (- (Math|Float|Truncate (LocalVariables|Get_GridSize)) 1))
          (LocalVariables|Set_Column _index_2)
          (bind (_outhit _returnvalue_5) (Collision|LineTraceByChannel (- (+ (Math|Vector|MakeVector (* (+ (Math|Random|RandomFloatinRangefromStream (* (LocalVariables|Get_MaxOffset) -1.0) (LocalVariables|Get_MaxOffset) (LocalVariables|Get_StreamX)) (+ (* (LocalVariables|Get_CellSize) (LocalVariables|Get_Column)) (* (LocalVariables|Get_CellSize) 0.5))) _returnvalue) (* (+ (Math|Random|RandomFloatinRangefromStream (* (LocalVariables|Get_MaxOffset) -1.0) (LocalVariables|Get_MaxOffset) (LocalVariables|Get_StreamY)) (+ (* (LocalVariables|Get_CellSize) (LocalVariables|Get_Row)) (* (LocalVariables|Get_CellSize) 0.5))) _returnvalue) (Variables|Default|GetGroundAltitude)) (Transformation|GetActorLocation (Components|GetOwner))) (Math|Vector|MakeVector _returnvalue_4 _returnvalue_4 0.0)) (+ (- (+ (Math|Vector|MakeVector (* (+ (Math|Random|RandomFloatinRangefromStream (* (LocalVariables|Get_MaxOffset) -1.0) (LocalVariables|Get_MaxOffset) (LocalVariables|Get_StreamX)) (+ (* (LocalVariables|Get_CellSize) (LocalVariables|Get_Column)) (* (LocalVariables|Get_CellSize) 0.5))) _returnvalue) (* (+ (Math|Random|RandomFloatinRangefromStream (* (LocalVariables|Get_MaxOffset) -1.0) (LocalVariables|Get_MaxOffset) (LocalVariables|Get_StreamY)) (+ (* (LocalVariables|Get_CellSize) (LocalVariables|Get_Row)) (* (LocalVariables|Get_CellSize) 0.5))) _returnvalue) (Variables|Default|GetGroundAltitude)) (Transformation|GetActorLocation (Components|GetOwner))) (Math|Vector|MakeVector _returnvalue_4 _returnvalue_4 0.0)) (Math|Vector|MakeVector 0.0 0.0 (Variables|Default|GetLinetraceLength))) "TraceTypeQuery1" false 0 "None" false "(R=1.000000,G=0.000000,B=0.000000,A=1.000000)" "(R=0.000000,G=1.000000,B=0.000000,A=1.000000)" 555.0))
          (Utilities|FlowControl|Sequence
            (:then_0
              (Math|Integer|IncrementInt (LocalVariables|Get_SpawnPointIndex)
                (:%20%20
                  (LocalVariables|Set_StreamX (Math|Random|MakeRandomStream (Class|KismetMathLibrary|RandomIntegerfromStream 2147483647 (Math|Random|MakeRandomStream (Class|KismetMathLibrary|RandomIntegerfromStream 2147483647 (Math|Random|MakeRandomStream (+ _returnvalue_2 __spawnpointindex)))))))
                  (LocalVariables|Set_StreamY (Math|Random|MakeRandomStream (Class|KismetMathLibrary|RandomIntegerfromStream 2147483647 (Math|Random|MakeRandomStream (Class|KismetMathLibrary|RandomIntegerfromStream 2147483647 (Math|Random|MakeRandomStream (- _returnvalue_2 __spawnpointindex))))))))))
            (:then_1
              (if _returnvalue_5
                (if (CallFunction|ContainsTags (Variables|/Script/Engine.Actor|GetTags (.HitActor (Collision|BreakHitResult _outhit))) (Variables|Default|GetCollisionTags))
                  (if (< (Class|KismetMathLibrary|DegAcos (Math|Vector|DotProduct (.ImpactNormal (Collision|BreakHitResult _outhit)) "0, 0,1.000000")) 35.0) ; If floor slope is < 35
                    (bind _returnvalue_6 (Game|SpawnActorfromClass :Class "/Game/Blueprints/ResourceSystem/ResourceActor.ResourceActor_C" :SpawnTransform (Math|Transform|MakeTransform (.ImpactPoint (Collision|BreakHitResult _outhit)) (Math|Rotator|MakeRotator 0.0 0.0 (Math|Random|RandomFloatinRangefromStream -359.0 359.0 (LocalVariables|Get_StreamX))) "1.000000,1.000000,1.000000") :CollisionHandlingOverride "AlwaysSpawn" :DA_Resource DA_Resource :ResourceSize (Math|Random|RandomIntegerinRangefromStream (.min ResourceSize) (.max ResourceSize) (LocalVariables|Get_StreamY)) :SM_Variety (Math|Random|RandomIntegerinRangefromStream (.min SM_Variety) (.max SM_Variety) (LocalVariables|Get_StreamX)) :Instigator 0))
                    (Transformation|AttachActorToActor _returnvalue_6 (Components|GetOwner) "None" "KeepWorld" "KeepWorld" "KeepWorld" true)
                    (Utilities|Array|Add (Variables|Default|GetResources) _returnvalue_6)))))))))
    (:then_1
      (Math|Integer|IncrementInt (Variables|Default|GetGenerations)))))