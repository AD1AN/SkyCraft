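; InteractSystem is an actor component that defines an actor's interact keys and tracks the prolonged interactions pawns have running on it.
; Helper functions look up key settings and check whether a player form is allowed for a key.
; AddProlonged and RemoveProlonged maintain the active list, enabling tick only while it has entries.
; Tick calls ServerInterrupt and drops any entry whose pawn moves beyond a fixed distance from the owner.
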(event EventTick
  (params (DeltaSeconds :type Float%20%28single-precision%29))
  (if (Utilities|Array|IsEmpty (Variables|Interact|GetCurrentProlonged))
    (Components|Tick|SetComponentTickEnabled false)
    (else
      (for (_array_element _array_index) (Variables|Interact|GetCurrentProlonged)
        (if (> (Math|Vector|Distance(Vector) (Transformation|GetActorLocation (Components|GetOwner)) (Transformation|GetActorLocation (.InteractedPawn (Utilities|Struct|BreakS_CurrentProlonged _array_element)))) 3e+02)
          (Default|ServerInterrupt (.InteractedPP_Sky (Utilities|Struct|BreakS_CurrentProlonged _array_element)) (Components|GetOwner) "NewEnumerator1" (.InteractKey (Utilities|Struct|BreakS_CurrentProlonged _array_element)) (.InteractedPawn (Utilities|Struct|BreakS_CurrentProlonged _array_element)) (.InteractedPC_Sky (Utilities|Struct|BreakS_CurrentProlonged _array_element)) (.InteractedPP_Sky (Utilities|Struct|BreakS_CurrentProlonged _array_element)))
          (Utilities|Array|RemoveIndex (Variables|Interact|GetCurrentProlonged) _array_index))))))

(fn FindInteractKey
  (params (InteractKey :type E_InteractKey%20Enum :default "NewEnumerator0"))
  (for _array_element (Variables|Interact|GetInteractKeys)
    (if (Utilities|Enum|Equal(Enum) (Utilities|Struct|BreakS_InteractKeySettings _array_element) InteractKey)
      (return true _array_element)))
  (return false ""))

(fn CheckInteractPlayerForm
  (params (KeySettings :type S%20Interact%20Key%20Settings%20Structure%20%28by%20ref%29) (PlayerForm :type E_PlayerForm%20Enum :default "NewEnumerator0"))
  (for _array_element (.PlayerForm (Utilities|Struct|BreakS_InteractKeySettings KeySettings))
    (if (Utilities|Enum|Equal(Enum) _array_element PlayerForm)
      (return true)))
  (return false))

(fn AddProlonged
  (params (InteractKey :type E_InteractKey%20Enum :default "NewEnumerator0") (InteractedPawn :type Pawn%20Object%20Reference) (InteractedPC_Sky :type PC%20Sky%20Object%20Reference) (InteractedPP_Sky :type PP%20Sky%20Object%20Reference))
  (Utilities|Array|Add (Variables|Interact|GetCurrentProlonged) (Utilities|Struct|MakeS_CurrentProlonged InteractKey InteractedPawn InteractedPC_Sky InteractedPP_Sky))
  (Components|Tick|SetComponentTickEnabled true))

(fn RemoveProlonged
  (params (InteractedPawn :type Pawn%20Object%20Reference))
  (bind _currentprolonged (Variables|Interact|GetCurrentProlonged))
  (for (_array_element _array_index) (Variables|Interact|GetCurrentProlonged)
    (if (== (Utilities|Struct|BreakS_CurrentProlonged _array_element) InteractedPawn)
      (Utilities|Array|RemoveIndex _currentprolonged _array_index)
      (if (Utilities|Array|IsEmpty _currentprolonged)
        (Components|Tick|SetComponentTickEnabled false))
      (return))))