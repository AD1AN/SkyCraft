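; World game mode that ties Ultra Dynamic Sky state to world save/load and manages players entering and leaving.
; Logout announces the departure, saves the player and destroys pawns according to player form; another event disconnects all connected clients.
; Astral actors are found or spawned per island, spaced along X at high altitude.
; New players are born as crystal pawns with creator-tagged starter equipment, attached to their island and possessed.
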(event Custom|DisconnectAllClients
  (for _array_element (Variables|/Script/SkyCraft.GSS|GetConnectedPlayers (Variables|Default|GetBP_GSS))
    (bind _asbp_pss (Utilities|Casting|CastToBP_PSS _array_element))
    (Default|ClientDisconnect _asbp_pss)))

(event EventOnLogout
  (params (ExitingController :type Controller%20Object%20Reference))
  (bind _asbp_pcs (Utilities|Casting|CastToBP_PCS ExitingController))
  (Variables|Default|SetLogoutPCS _asbp_pcs)
  (Class|GMS|SendMessageWorld (Class|AdvancedSessionsLibrary|GetPlayerName (Variables|Default|GetLogoutPCS)) "left the world.")
  (Class|PSS|SavePlayer (Variables|/Script/SkyCraft.PCS|GetPSS (Variables|Default|GetLogoutPCS)))
  (switch Utilities|FlowControl|Switch|SwitchonEPlayerForm (Variables|/Script/SkyCraft.PSS|GetPlayerForm (Variables|/Game/Blueprints/BP_PCS.BP_PCS_C|GetBP_PSS (Variables|Default|GetLogoutPCS)))
    (:Crystal
      (Actor|DestroyActor (Variables|/Game/Blueprints/BP_PSS.BP_PSS_C|GetPF_Crystal (Variables|/Game/Blueprints/BP_PCS.BP_PCS_C|GetBP_PSS (Variables|Default|GetLogoutPCS)))))
    (:Normal
      (Utilities|IsValid (Variables|/Game/Blueprints/PF_Normal.PF_Normal_C|GetPF_Phantom (Variables|/Game/Blueprints/BP_PSS.BP_PSS_C|GetPF_Normal (Variables|/Game/Blueprints/BP_PCS.BP_PCS_C|GetBP_PSS (Variables|Default|GetLogoutPCS)))) :!label _label
        (:Is%20Valid
          (Actor|DestroyActor (Variables|/Game/Blueprints/PF_Normal.PF_Normal_C|GetPF_Phantom (Variables|/Game/Blueprints/BP_PSS.BP_PSS_C|GetPF_Normal (Variables|/Game/Blueprints/BP_PCS.BP_PCS_C|GetBP_PSS (Variables|Default|GetLogoutPCS))))))
        (:Is%20Not%20Valid
          _))
      (Actor|DestroyActor (Variables|/Game/Blueprints/BP_PSS.BP_PSS_C|GetPF_Normal (Variables|/Game/Blueprints/BP_PCS.BP_PCS_C|GetBP_PSS (Variables|Default|GetLogoutPCS)))))
    (:Phantom
      (if (Variables|/Script/SkyCraft.PlayerPhantom|GetbEstrayPhantom (Variables|/Game/Blueprints/BP_PSS.BP_PSS_C|GetPF_Spirit (Variables|/Game/Blueprints/BP_PCS.BP_PCS_C|GetBP_PSS (Variables|Default|GetLogoutPCS))))
        (Actor|DestroyActor (Variables|/Game/Blueprints/BP_PSS.BP_PSS_C|GetPF_Spirit (Variables|/Game/Blueprints/BP_PCS.BP_PCS_C|GetBP_PSS (Variables|Default|GetLogoutPCS))))
        (else
          (goto _label))))
    (:Dead
      (Actor|DestroyActor (Variables|/Game/Blueprints/BP_PSS.BP_PSS_C|GetPF_Dead (Variables|/Game/Blueprints/BP_PCS.BP_PCS_C|GetBP_PSS (Variables|Default|GetLogoutPCS)))))))

(event EventSaveWorld
  (Variables|/Game/Blueprints/BP_WorldSave.BP_WorldSave_C|SetUDS_And_UDW (Variables|Default|GetBP_WorldSave) (Default|CreateUDSandUDWStateforSaving (Variables|Default|GetUDS)))
  (|CallParentFunction))

(event EventLoadWorld
  (bind _asbp_world_save (Utilities|Casting|CastToBP_WorldSave (Variables|Default|GetWorldSave)))
  (bind _output_get (Variables|Default|SetBP_WorldSave _asbp_world_save))
  (if (Variables|/Script/SkyCraft.WorldSave|GetbFirstTimeLoadingWorld _output_get)
    _
    (else
      (Default|ApplySavedUDSandUDWState (Variables|Default|GetUDS) (Variables|/Game/Blueprints/BP_WorldSave.BP_WorldSave_C|GetUDS_And_UDW (Variables|Default|GetBP_WorldSave)))))
  (|CallParentFunction))

(event EventStartWorld
  (bind _asbp_gis (Utilities|Casting|CastToBP_GIS (Game|GetGameInstance)))
  (Variables|Default|SetBP_GIS _asbp_gis)
  (bind _asbp_gss (Utilities|Casting|CastToBP_GSS (Game|GetGameState)))
  (bind _output_get (Variables|Default|SetBP_GSS _asbp_gss))
  (Variables|/Game/Blueprints/BP_GSS.BP_GSS_C|SetBP_GMS _output_get self)
  (bind _returnvalue (Actor|GetActorOfClass "/Game/UltraDynamicSky/Blueprints/Ultra_Dynamic_Sky.Ultra_Dynamic_Sky_C"))
  (Variables|Default|SetUDS _returnvalue)
  (|CallParentFunction))

(fn ConstructionScript)

(fn CreateAstral
  (params (Island :type Island%20Object%20Reference))
  (bind _islands (Variables|Astral|GetIslands))
  (bind _returnvalue (Utilities|Array|LastIndex _islands))
  (if (!= _returnvalue 0)
    (bind _index (Utilities|FlowControl|ForLoopwithBreak 0 _returnvalue)
      (:LoopBody
        (if (not (== (* _index 200000) (.x (Transformation|GetActorLocation (Utilities|Array|Get(acopy) (Variables|Astral|GetIslands) _index)))))
          (bind _returnvalue_2 (Game|SpawnActorfromClass "/Game/Blueprints/Astral.Astral_C" (Math|Transform|MakeTransform (Math|Vector|MakeVector (* _index 200000) 0.0 1e+08) "0, 0, 0" "1.000000,1.000000,1.000000") "AlwaysSpawn" "OverrideRootScale" 0 Island 0))
          (Utilities|Array|Add (Variables|Astral|GetIslands) Island)
          (Utilities|Array|Add (Variables|Astral|GetAstrals) _returnvalue_2)
          (return _returnvalue_2)))
      (:Completed
        (bind _returnvalue_3 (Game|SpawnActorfromClass "/Game/Blueprints/Astral.Astral_C" (Math|Transform|MakeTransform (Math|Vector|MakeVector (* (Utilities|Array|Length _islands) 200000) 0.0 1e+08) "0, 0, 0" "1.000000,1.000000,1.000000") "AlwaysSpawn" "OverrideRootScale" 0 Island 0 :!label _label))
        (Utilities|Array|Add (Variables|Astral|GetIslands) Island)
        (Utilities|Array|Add (Variables|Astral|GetAstrals) _returnvalue_3)
        (return _returnvalue_3)))
    (else
      (goto _label))))

(fn Find/CreateAstral
  (params (Island :type Island%20Object%20Reference))
  (for (_array_element _array_index) (Variables|Astral|GetIslands)
    (if (== _array_element Island)
      (return (Utilities|Array|Get(acopy) (Variables|Astral|GetAstrals) _array_index))))
  (bind _astral (Astral|CreateAstral Island))
  (return _astral))

(fn BornPlayerCrystal
  (params (PCS :type PCS%20Object%20Reference))
  (bind _returnvalue (Game|SpawnActorfromClass "/Game/Blueprints/PF_Crystal.PF_Crystal_C" (Math|Transform|MakeTransform "0, 0, 0" "0, 0, 0" "1.000000,1.000000,1.000000") "AlwaysSpawn" "MultiplyWithRoot" PCS (Variables|/Script/SkyCraft.PCS|GetPSS PCS) 0))
  (LocalVariables|Set_spawned_PF_Island _returnvalue)
  (for _index (range 0 3)
    (Utilities|IsValid (Utilities|Select :Index _index :Option%200 0 :Option%201 "/Game/DataAssets/Item/I_EQOutfit_OldNosha.I_EQOutfit_OldNosha" :Option%202 0 :Option%203 "/Game/DataAssets/Item/I_EQFeet_OldNosha.I_EQFeet_OldNosha")
      (:Is%20Valid
        (if (.Has (CallFunction|ContainsProperty (Variables|/Script/SkyCraft.DA_Item|GetInitialProperties (Utilities|Select :Index _index :Option%200 0 :Option%201 "/Game/DataAssets/Item/I_EQOutfit_OldNosha.I_EQOutfit_OldNosha" :Option%202 0 :Option%203 "/Game/DataAssets/Item/I_EQFeet_OldNosha.I_EQFeet_OldNosha")) "/Game/DataAssets/ItemProperty/Creator.Creator"))
          (Utilities|Struct|SetmembersinItemProperty (Utilities|Array|Get(acopy) (Variables|/Script/SkyCraft.DA_Item|GetInitialProperties (Utilities|Select :Index _index :Option%200 0 :Option%201 "/Game/DataAssets/Item/I_EQOutfit_OldNosha.I_EQOutfit_OldNosha" :Option%202 0 :Option%203 "/Game/DataAssets/Item/I_EQFeet_OldNosha.I_EQFeet_OldNosha")) (.Index (CallFunction|ContainsProperty (Variables|/Script/SkyCraft.DA_Item|GetInitialProperties (Utilities|Select :Index _index :Option%200 0 :Option%201 "/Game/DataAssets/Item/I_EQOutfit_OldNosha.I_EQOutfit_OldNosha" :Option%202 0 :Option%203 "/Game/DataAssets/Item/I_EQFeet_OldNosha.I_EQFeet_OldNosha")) "/Game/DataAssets/ItemProperty/Creator.Creator"))) (Utilities|Array|MakeArray (Variables|/Script/SkyCraft.PSS|GetSteamID (Variables|/Script/SkyCraft.PCS|GetPSS PCS)))))
        (Utilities|Array|SetArrayElem (Variables|/Script/SkyCraft.InventoryComponent|GetSlots (Variables|/Script/SkyCraft.PlayerCrystal|GetEquipmentInventoryComponent (LocalVariables|Get_spawned_PF_Island))) _index (Utilities|Struct|MakeSlot (Utilities|Select :Index _index :Option%200 0 :Option%201 "/Game/DataAssets/Item/I_EQOutfit_OldNosha.I_EQOutfit_OldNosha" :Option%202 0 :Option%203 "/Game/DataAssets/Item/I_EQFeet_OldNosha.I_EQFeet_OldNosha") 1 (Variables|/Script/SkyCraft.DA_Item|GetInitialProperties (Utilities|Select :Index _index :Option%200 0 :Option%201 "/Game/DataAssets/Item/I_EQOutfit_OldNosha.I_EQOutfit_OldNosha" :Option%202 0 :Option%203 "/Game/DataAssets/Item/I_EQFeet_OldNosha.I_EQFeet_OldNosha")))))))
  (Transformation|AttachActorToActor (LocalVariables|Get_spawned_PF_Island) (Variables|/Script/SkyCraft.PSS|GetPlayerIsland (Variables|/Script/SkyCraft.PCS|GetPSS PCS)) "None" "KeepRelative" "KeepWorld" "KeepWorld" true)
  (Pawn|Possess PCS (LocalVariables|Get_spawned_PF_Island))
  (return (LocalVariables|Get_spawned_PF_Island)))