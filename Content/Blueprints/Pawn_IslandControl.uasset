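; Pawn a player possesses to steer a flying island (IslandArchon), while their character form is held in a spirit-machine state.
; Look-relative movement and vertical inputs go through server RPCs to set island direction and altitude, and Tick clamps island height.
; Client events handle the control widget, Niagara direction effects and sound.
; Exiting passes look rotation to the original pawn, blends the camera back and repossesses it.
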(event Custom|Server_SetTargetDirection
  (params (TargetDirection :type Vector))
  (bind _islandarchon (Variables|Default|GetIslandArchon))
  (Variables|/Game/Blueprints/IslandArchon.IslandArchon_C|SetTargetDirection _islandarchon TargetDirection)
  (Variables|/Game/Blueprints/IslandArchon.IslandArchon_C|SetCDT _islandarchon (Variables|/Game/Blueprints/IslandArchon.IslandArchon_C|GetFly_CDT _islandarchon))
  (Default|ChangeStopIsland (Variables|Default|GetIslandArchon) false)
  (CallFunction|ClientSetTargetDirectionFX (Variables|/Game/Blueprints/IslandArchon.IslandArchon_C|GetTargetDirection (Variables|Default|GetIslandArchon))))

(event Custom|HideCompleted
  (Widget|RemovefromParent (Variables|Default|GetW_PawnIslandControl)))

(event Custom|Server_VerticalInput:Altitude
  (params (Altitude :type Float%20%28double-precision%29))
  (bind _islandarchon (Variables|Default|GetIslandArchon))
  (bind _output_get (Variables|/Game/Blueprints/IslandArchon.IslandArchon_C|SetAltitude _islandarchon Altitude))
  (Variables|/Game/Blueprints/IslandArchon.IslandArchon_C|SetTargetAltitude _islandarchon (+ _output_get (.z (Transformation|GetActorLocation _islandarchon)))))

(event Custom|Multicast_PossessControlPawn
  (params (PawnInControl :type Pawn%20Object%20Reference) (PP_SkyInControl :type BP%20PAI%20Object%20Reference))
  (bind _pf_normal (Variables|/Game/Blueprints/BP_PAI.BP_PAI_C|GetPF_Normal PP_SkyInControl))
  (bind _abp_normal (Variables|/Game/Blueprints/PF_Normal.PF_Normal_C|GetABP_Normal _pf_normal))
  (Variables|Default|SetPawnInControl PawnInControl)
  (Variables|Default|SetBP_PAI_InControl PP_SkyInControl)
  (switch Utilities|FlowControl|Switch|SwitchonEPlayerForm (Variables|/Game/Blueprints/BP_PAI.BP_PAI_C|GetCurrentPF PP_SkyInControl)
    (:Normal
      (Variables|/Game/Characters/ABP_Normal.ABP_Normal_C|SetuseSpiritMachine _abp_normal true)
      (Variables|/Game/Blueprints/PF_Normal.PF_Normal_C|SetinSpiritAnim _pf_normal true)
      (Variables|/Game/Characters/ABP_Normal.ABP_Normal_C|SetLookAt _abp_normal false)
      (Variables|/Game/Blueprints/PF_Normal.PF_Normal_C|SetcanMove _pf_normal false)
      (Variables|/Game/Blueprints/PF_Normal.PF_Normal_C|SetcanQSPressing _pf_normal false)
      (Variables|/Game/Blueprints/PF_Normal.PF_Normal_C|SetcanQSScrolling _pf_normal false)
      (Variables|/Game/Blueprints/PF_Normal.PF_Normal_C|SetcanInteract _pf_normal false)
      (Default|SetQSI _pf_normal -1))))

(event Custom|TargetDirectionChanged_Event_0
  (bind _islandarchon (Variables|Default|GetIslandArchon))
  (Niagara|SetNiagaraVariable(Vector3) (Variables|/Game/Blueprints/IslandArchon.IslandArchon_C|GetSN_Outside _islandarchon) "AttractorPosition" (Math|Vector|SelectVector "0, 0, 0" (* (Variables|/Game/Blueprints/IslandArchon.IslandArchon_C|GetTargetDirection _islandarchon) 3e+03) (Variables|/Game/Blueprints/IslandArchon.IslandArchon_C|GetStopIsland _islandarchon))))

(event Custom|Server_SetAltitudeSetted
  (Variables|/Game/Blueprints/IslandArchon.IslandArchon_C|SetAltitudeSetted (Variables|Default|GetIslandArchon) false))

(event Custom|Multicast_UnpossessControlPawn
  (Utilities|FlowControl|Sequence
    (:then_0
      (switch Utilities|FlowControl|Switch|SwitchonEPlayerForm (Variables|/Game/Blueprints/BP_PAI.BP_PAI_C|GetCurrentPF (Variables|Default|GetBP_PAI_InControl))
        (:Normal
          (Variables|/Game/Blueprints/PF_Normal.PF_Normal_C|SetinSpiritAnim (Variables|/Game/Blueprints/BP_PAI.BP_PAI_C|GetPF_Normal (Variables|Default|GetBP_PAI_InControl)) false))))
    (:then_1
      (Variables|Default|SetBP_PAI_InControl 0) ; Empty
      (Variables|Default|SetPawnInControl 0) ; Empty
    )))

(event Custom|Server_ReturnToPF
  (params (LookRotation :type Rotator))
  (Class|BPILookRotation|SetLookRotation(Message) (Variables|Default|GetPawnInControl) LookRotation)
  (Game|Player|SetViewTargetwithBlend (Variables|/Game/Blueprints/BP_PAI.BP_PAI_C|GetBP_PCS (Variables|Default|GetBP_PAI_InControl)) (Variables|Default|GetPawnInControl) 1.0 "VTBlend_EaseInOut" 2.0 false)
  (Default|PossessPawn (Variables|/Game/Blueprints/BP_PAI.BP_PAI_C|GetBP_PCS (Variables|Default|GetBP_PAI_InControl)) (Variables|Default|GetPawnInControl) true)
  (CallFunction|MulticastUnpossessControlPawn))

(event Custom|Client_ReturnToPF
  (CallFunction|ServerCallMulticastSetLookRotation (Variables|Default|GetLookRotation))
  (CallFunction|ServerReturntoPF (Variables|Default|GetLookRotation)))

(event Custom|Client_Possessed
  (bind _islandarchon (Variables|Default|GetIslandArchon))
  (bind _islandarchon_2 (Variables|Default|GetIslandArchon))
  (Actor|Tick|SetActorTickEnabled true)
  (bind _returnvalue (UserInterface|CreateWidget "/Game/Widgets/W_PawnIslandControl.W_PawnIslandControl_C" 0 (Variables|Default|GetIslandArchon) (Variables|Default|GetBP_PAI_InControl)))
  (bind _output_get (Variables|Default|SetW_PawnIslandControl _returnvalue))
  (UserInterface|Animation|PlayAnimation _output_get (Variables|/Game/Widgets/W_PawnIslandControl.W_PawnIslandControl_C|Getanim_show _output_get) 0.0 1 "Forward" 1.0 false)
  (UserInterface|Viewport|AddtoViewport _output_get 0)
  (Components|Activation|SetActive (Variables|/Game/Blueprints/IslandArchon.IslandArchon_C|GetSN_Outside (Variables|Default|GetIslandArchon)) true false)
  (EventDispatchers|AssignOnTargetDirectionChanged _islandarchon (delegate Custom|TargetDirectionChanged_Event_0))
  (EventDispatchers|BindEventtoOnStopIslandChange _islandarchon (delegate Custom|TargetDirectionChanged_Event_0))
  (Niagara|SetNiagaraVariable(Vector3) (Variables|/Game/Blueprints/IslandArchon.IslandArchon_C|GetSN_Outside _islandarchon_2) "AttractorPosition" (Math|Vector|SelectVector "0, 0, 0" (* (Variables|/Game/Blueprints/IslandArchon.IslandArchon_C|GetTargetDirection _islandarchon_2) 3e+03) (Variables|/Game/Blueprints/IslandArchon.IslandArchon_C|GetStopIsland _islandarchon_2))))

(event Custom|Client_SetTargetDirectionFX
  (params (TargetDirection :type Vector))
  (Niagara|SpawnSystemAttached "/Game/Niagara/NS_IA_DirectionFire.NS_IA_DirectionFire" (Variables|/Script/Engine.Actor|GetRootComponent (Variables|Default|GetIslandArchon)) "None" "0, 0, 0" (Math|Rotator|MakeRotator 0.0 0.0 (.yaw (Math|Conversions|RotationFromXVector TargetDirection))) "KeepRelativeOffset" true)
  (Audio|PlaySound2D "/Game/Audio/SFX/IA_Direction.IA_Direction" 1.0 1.0 0.0 0 0)
  (Default|CallSetDirection))

(event Custom|Multicast_SetLookRotation
  (params (LookRotation :type Rotator))
  (bind _output_get (Variables|Default|SetLookRotation LookRotation))
  (Transformation|SetWorldRotation (Variables|Default|GetCameraBoom) _output_get false false))

(event Custom|Server_CallMulticastSetLookRotation
  (params (LookRotation :type Rotator))
  (CallFunction|MulticastSetLookRotation LookRotation))

(event Input|EnhancedActionEvents|EnhancedInputActionInteract1
  (params (ActionValue :type Boolean) (ElapsedSeconds :type Float%20%28double-precision%29) (TriggeredSeconds :type Float%20%28double-precision%29) (InputAction :type Input%20Action%20Object%20Reference :default "/Game/Misc/EnhancedInput/Interact1.Interact1"))
  (:Started
    (Default|CreateMenu (Variables|Default|GetIslandArchon) self (Variables|Default|GetBP_PAI_InControl))
    (Input|DisableInput (Variables|/Game/Blueprints/BP_PAI.BP_PAI_C|GetBP_PCS (Variables|Default|GetBP_PAI_InControl)))))

(event Input|EnhancedActionEvents|EnhancedInputActionDropItem
  (params (ActionValue :type Boolean) (ElapsedSeconds :type Float%20%28double-precision%29) (TriggeredSeconds :type Float%20%28double-precision%29) (InputAction :type Input%20Action%20Object%20Reference :default "/Game/Misc/EnhancedInput/DropItem.DropItem"))
  (:Started
    (CallFunction|ClientReturntoPF)))

(event Input|EnhancedActionEvents|EnhancedInputActionSpiritForm
  (params (ActionValue :type Boolean) (ElapsedSeconds :type Float%20%28double-precision%29) (TriggeredSeconds :type Float%20%28double-precision%29) (InputAction :type Input%20Action%20Object%20Reference :default "/Game/Misc/EnhancedInput/SpiritForm.SpiritForm"))
  (:Started
    (Default|ServerToggleStopIA (Variables|Default|GetBP_PAI_InControl))))

(event Input|EnhancedActionEvents|EnhancedInputActionCameraRotate
  (params (ActionValue :type Vector%202D%20Structure) (ElapsedSeconds :type Float%20%28double-precision%29) (TriggeredSeconds :type Float%20%28double-precision%29) (InputAction :type Input%20Action%20Object%20Reference :default "/Game/Misc/EnhancedInput/CameraRotate.CameraRotate"))
  (bind (_x _y) (Math|Vector2D|BreakVector2D ActionValue))
  (bind _bp_sgi (Variables|Default|GetBP_SGI))
  (bind _customsettings (Variables|/Game/Blueprints/BP_SGI.BP_SGI_C|GetCustomSettings _bp_sgi))
  (bind _camerasensetivity (Variables|/Game/Blueprints/CustomSettingsSave.CustomSettingsSave_C|GetCameraSensetivity _customsettings))
  (Variables|Default|SetLookRotation (Math|Rotator|MakeRotator (.roll (Variables|Default|GetLookRotation)) (Math|Float|ClampAngle (+ (* _y _camerasensetivity) (.pitch (Variables|Default|GetLookRotation))) -5e+01 0.0) (+ (* _x _camerasensetivity) (.yaw (Variables|Default|GetLookRotation))))))

(event Input|EnhancedActionEvents|EnhancedInputActionLMB
  (params (ActionValue :type Boolean) (ElapsedSeconds :type Float%20%28double-precision%29) (TriggeredSeconds :type Float%20%28double-precision%29) (InputAction :type Input%20Action%20Object%20Reference :default "/Game/Misc/EnhancedInput/LMB.LMB"))
  (:Started
    (CallFunction|ServerSetTargetDirection (Math|Vector|GetForwardVector (Math|Rotator|MakeRotator 0.0 0.0 (.yaw (Variables|Default|GetLookRotation)))))))

(event Input|EnhancedActionEvents|EnhancedInputActionMoveVertical
  (params (ActionValue :type Float%20%28double-precision%29) (ElapsedSeconds :type Float%20%28double-precision%29) (TriggeredSeconds :type Float%20%28double-precision%29) (InputAction :type Input%20Action%20Object%20Reference :default "/Game/Misc/EnhancedInput/MoveVertical.MoveVertical"))
  (:Triggered
    (if (not (Variables|/Game/Blueprints/IslandArchon.IslandArchon_C|GetAltitudeSetted (Variables|Default|GetIslandArchon)))
      (CallFunction|ServerVerticalInput:Altitude (* ActionValue 5e+01))))
  (:Started
    (CallFunction|ServerSetAltitudeSetted)))

(event Input|EnhancedActionEvents|EnhancedInputActionMove2D
  (params (ActionValue :type Vector%202D%20Structure) (ElapsedSeconds :type Float%20%28double-precision%29) (TriggeredSeconds :type Float%20%28double-precision%29) (InputAction :type Input%20Action%20Object%20Reference :default "/Game/Misc/EnhancedInput/Move2D.Move2D"))
  (bind (_x _y) (Math|Vector2D|BreakVector2D ActionValue))
  (bind _lookrotation (Variables|Default|GetLookRotation))
  (:Triggered
    (Utilities|FlowControl|DoOnce false :!label _label
      (:Completed
        (CallFunction|ServerSetTargetDirection (+ (* (Math|Vector|GetRightVector (Math|Rotator|MakeRotator 0.0 0.0 (.yaw _lookrotation))) _x) (* (Math|Vector|GetForwardVector (Math|Rotator|MakeRotator 0.0 0.0 (.yaw _lookrotation))) _y))))))
  (:Completed
    (goto _label Reset)))

(event EventBeginPlay
  (bind _asbp_sgi (Utilities|Casting|CastToBP_SGI (Game|GetGameInstance)))
  (Variables|Default|SetBP_SGI _asbp_sgi))

(event EventTick
  (params (DeltaSeconds :type Float%20%28single-precision%29))
  (bind _islandarchon (Variables|Default|GetIslandArchon))
  (bind _islandarchon_2 (Variables|Default|GetIslandArchon))
  (bind _returnvalue (Transformation|GetActorLocation _islandarchon_2))
  (bind _returnvalue_2 (Transformation|GetActorLocation _islandarchon))
  (Utilities|FlowControl|Sequence
    (:then_0
      (Transformation|SetWorldRotation (Variables|Default|GetCameraBoom) (Variables|Default|GetLookRotation) false false))
    (:then_1
      (Utilities|FlowControl|Sequence
        (:then_0
          (if (> (.z _returnvalue) 3e+04)
            (Variables|/Game/Blueprints/IslandArchon.IslandArchon_C|SetAltitude _islandarchon 0.0)
            (Transformation|SetActorLocation _islandarchon (Math|Vector|MakeVector (.x _returnvalue_2) (.y _returnvalue_2) 3e+04) false false)))
        (:then_1
          (if (< (.z _returnvalue) 5e+03)
            (Variables|/Game/Blueprints/IslandArchon.IslandArchon_C|SetAltitude _islandarchon 0.0)
            (Transformation|SetActorLocation _islandarchon (Math|Vector|MakeVector (.x _returnvalue_2) (.y _returnvalue_2) 5e+03) false false)))))))

(event EventPossessed
  (params (NewController :type Controller%20Object%20Reference))
  (CallFunction|ClientPossessed)
  (Actor|Tick|SetActorTickEnabled true)
  (Game|Player|SetViewTargetwithBlend (Variables|/Game/Blueprints/BP_PAI.BP_PAI_C|GetBP_PCS (Variables|Default|GetBP_PAI_InControl)) self 0.0 "VTBlend_Linear" 0.0 false))

(event EventClientUnpossess
  (bind _w_pawnislandcontrol (Variables|Default|GetW_PawnIslandControl))
  (bind _anim_hide (Variables|/Game/Widgets/W_PawnIslandControl.W_PawnIslandControl_C|Getanim_hide _w_pawnislandcontrol))
  (Class|UserWidget|BindtoAnimationFinished _w_pawnislandcontrol _anim_hide (delegate Custom|HideCompleted))
  (UserInterface|Animation|PlayAnimation _w_pawnislandcontrol _anim_hide 0.0 1 "Forward" 1.0 false)
  (Components|Activation|SetActive (Variables|/Game/Blueprints/IslandArchon.IslandArchon_C|GetSN_Outside (Variables|Default|GetIslandArchon)) false false)
  (EventDispatchers|UnbindallEventsfromOnTargetDirectionChanged (Variables|Default|GetIslandArchon)))

(event EventUnpossessed
  (params (OldController :type Controller%20Object%20Reference))
  (Actor|Tick|SetActorTickEnabled false))

(fn ConstructionScript)

(fn OnRepPawninControl
  (Default|CallCharinControlChanged))