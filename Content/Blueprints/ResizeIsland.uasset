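; ResizeIsland is a voxel world Blueprint that builds a procedurally generated island at a configurable size.
; On BeginPlay it binds to OnWorldLoaded and, if the world is not yet created, passes a fixed seed and IslandSize to the generator before calling CreateWorld.
; Generated sets IsGenerated and broadcasts OnGenerated.
; CheckIsGenerated rebroadcasts that event when generation has already finished.
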(event EventBeginPlay
  (bind _generator (Variables|Default|GetGenerator))
  (EventDispatchers|BindEventtoOnWorldLoaded (EventDispatchers|CreateEvent :!event Generated))
  (if (not (Class|VoxelWorld|IsCreated))
    (Class|VoxelGeneratorTools|SetGeneratorParameter _generator "SeedName" (Class|KismetSystemLibrary|MakeLiteralInteger))
    (Class|VoxelGeneratorTools|SetGeneratorParameter _generator "IslandSize" (Variables|Default|GetIslandSize))
    (Class|VoxelWorld|CreateWorld)))

(fn ConstructionScript)

(fn CheckIsGenerated
  (if (Variables|Default|GetisGenerated)
    (Default|CallOnGenerated)))

(fn Generated
  (Variables|Default|SetisGenerated true)
  (Default|CallOnGenerated))