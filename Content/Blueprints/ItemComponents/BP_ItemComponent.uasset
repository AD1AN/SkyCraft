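; BP_ItemComponent is a base component for item behaviour attached to a PF_Normal owner.
; On BeginPlay it casts the owner, caches it and its BPPAI reference, calls the empty StartItemComponent hook, then marks itself started.
; A wrong owner type only prints an error.
; EndPlay calls the empty EndItemComponent hook only if the component started, leaving both hooks for children to override.
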(event Custom|EndItemComponent)

(event Custom|StartItemComponent)

(event Custom|Started
  (Variables|Default|SetisStarted true))

(event EventBeginPlay
  (bind _aspf_normal (Utilities|Casting|CastToPF_Normal (Components|GetOwner))
    (:then
      (bind _output_get (Variables|Default|SetPF_Normal _aspf_normal))
      (Variables|Default|SetBP_PAI (Variables|/Game/Blueprints/PF_Normal.PF_Normal_C|GetBP_PAI _output_get))
      (CallFunction|StartItemComponent)
      (CallFunction|Started))
    (:CastFailed
      (Development|PrintString (Utilities|String|Append "ItemComponent: " (Utilities|GetDisplayName self) " owner of this component is not PF_Normal. Owner: " (Utilities|GetDisplayName (Components|GetOwner))) true true "(R=1.000000,G=0.000000,B=0.139065,A=1.000000)" 555.0))))

(event EventEndPlay
  (params (EndPlayReason :type EEndPlayReason%20Enum :default "Destroyed"))
  (if (Variables|Default|GetisStarted)
    (CallFunction|EndItemComponent)))