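; Chunk_Essence is a world chunk that fills its box with randomly placed BP_Essence actors on the server.
; BeginPlay chains four runs of a zero-delay loop macro to spread the spawns over time.
; Nested weighted rolls set each essence's RGB, mostly blue-dominant with rarer variants.
; When replicated HMPR drops to zero or below, the chunk removes itself from BPGMS's lists and destroys its essences and itself.
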(event EventBeginPlay
  (if (Networking|IsServer)
    (Utilities|LOOPEssence
      (:Completed
        (Utilities|LOOPEssence
          (:Completed
            (Utilities|LOOPEssence
              (:Completed
                (Utilities|LOOPEssence)))))))))

(fn ConstructionScript)

(fn DestroyChunk
  (bind _self self)
  (bind _bp_gms (Variables|Default|GetBP_GMS))
  (bind _bp_gms_2 (Variables|Default|GetBP_GMS))
  (bind _spawnedchunkessence (Variables|/Game/Blueprints/BP_GMS.BP_GMS_C|GetSpawnedChunkEssence _bp_gms_2))
  (bind _returnvalue (Utilities|Array|FindItem _spawnedchunkessence _self))
  (Utilities|Array|RemoveIndex (Variables|/Game/Blueprints/BP_GMS.BP_GMS_C|GetSpawnedChunkEssenceCoords _bp_gms) _returnvalue)
  (Utilities|Array|RemoveIndex (Variables|/Game/Blueprints/BP_GMS.BP_GMS_C|GetSpawnedChunkEssence _bp_gms) _returnvalue)
  (Utilities|FlowControl|Sequence
    (:then_0
      (for _array_element (Variables|Default|GetEssences)
        (Utilities|IsValid _array_element
          (:Is%20Valid
            (Default|DestroyEssence _array_element)))))
    (:then_1
      (Actor|DestroyActor))))

(fn OnRepHMPR
  (if (<= (Variables|Default|GetHMPR) 0)
    (CallFunction|DestroyChunk)))