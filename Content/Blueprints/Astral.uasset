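; Astral is an actor that populates its surroundings with a core and constellation actors when play begins.
; On the server only, it spawns an AstralCore above itself, passing itself as the core's Astral reference.
; It then walks the Island's constellation entries and spawns each valid actor class from the entry's constellation data, using the stored location offset from the Astral and the stored rotation.
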(event EventBeginPlay
  (if (Networking|IsServer)
    (Game|SpawnActorfromClass "/Game/Blueprints/AstralCore.AstralCore_C" (Math|Transform|MakeTransform (+ (Transformation|GetActorLocation) "0.000000,0.000000,250.000000") "0, 0, 0" "1.000000,1.000000,1.000000") "AlwaysSpawn" "MultiplyWithRoot" 0 self 0)
    (for _array_element (Variables|/Script/SkyCraft.Island|GetSS_Constellations (Variables|Default|GetIsland))
      (if (Utilities|IsValidClass (Variables|/Script/SkyCraft.DA_Constellation|GetActorClass (.DA_Constellation (Utilities|Struct|BreakSS_Constellation _array_element))))
        (Game|SpawnActorfromClass (Variables|/Script/SkyCraft.DA_Constellation|GetActorClass (.DA_Constellation (Utilities|Struct|BreakSS_Constellation _array_element))) (Math|Transform|MakeTransform (+ (.RelativeLocation (Utilities|Struct|BreakSS_Constellation _array_element)) (Transformation|GetActorLocation)) (.Rotation (Utilities|Struct|BreakSS_Constellation _array_element)) "1.000000,1.000000,1.000000") "AlwaysSpawn" "MultiplyWithRoot" 0 0)))))

(fn ConstructionScript)