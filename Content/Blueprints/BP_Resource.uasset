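; BP_Resource is a harvestable world resource, such as stone or a tree, configured by a DAResource data asset.
; ApplyDamage drains HealthSystem; at zero it rolls weighted CurrentSize loot into the dealer's inventory, plays a per-resource sound and destroys the actor.
; Server interaction instead rolls loot from the first size entry, destroying the actor when an inventory add succeeds.
; A separate multicast event plays sounds at random pitch.
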(event Custom|Multicast_PlaySound
  (params (Sound :type Sound%20Base%20Object%20Reference))
  (Audio|SpawnSoundatLocation Sound (Transformation|GetActorLocation) "0, 0, 0" 1.0 (Math|Random|RandomFloatinRange 0.75 1.2) 0.0 "/Game/Audio/NormalAttenuation.NormalAttenuation" 0))

(fn ConstructionScript)

(fn GetInteractLocation
  (return (Transformation|GetActorLocation)))

(fn GetInteractSystem
  (return (Variables|Default|GetInteractSystem)))

(fn GetSkyTags
  (return (Utilities|Struct|MakeGetSkyTagsOut (Variables|/Script/SkyCraft.SkyTags|GetDA_SkyTags (Variables|Default|GetSkyTags)))))

(fn ApplyDamage
  (params (In :type Apply%20Damage%20in%20Structure))
  (bind _healthsystem (Variables|Default|GetHealthSystem))
  (bind _output_get (Variables|/Script/SkyCraft.HealthSystem|SetHealth _healthsystem (- (Variables|/Script/SkyCraft.HealthSystem|GetHealth _healthsystem) (.basedamage In))))
  (if (<= _output_get 0)
    (bind _inventory (Class|BPIGetInventory|GetInventory(Message) (.damagedealer In)))
    (Utilities|IsValid _inventory
      (:Is%20Valid
        (for _array_element (Utilities|Struct|BreakResourceSize (Variables|Default|GetCurrentSize))
          (if (Math|Random|RandomBoolwithWeight (.Probability (Utilities|Struct|BreakResourceLoot _array_element)))
            (Default|AddtoInventory _inventory (Utilities|Struct|MakeInventorySlot (.Item (Utilities|Struct|BreakResourceLoot _array_element)) (Math|Random|RandomIntegerinRange (.Min (Utilities|Struct|BreakResourceLoot _array_element)) (.Max (Utilities|Struct|BreakResourceLoot _array_element))) 0)))))
      (:Is%20Not%20Valid
        _))
    (Audio|PlaySoundatLocation (.Value (Utilities|Map|Find (Utilities|Map|MakeMap "/Game/DataAssets/Resource/Stone.Stone" "/Game/Audio/SFX/HitStone/Meta_HitStone.Meta_HitStone" "/Game/DataAssets/Resource/KarkTree.KarkTree" "/Game/Audio/SFX/HitTree/TreeDestroy.TreeDestroy") (Variables|Default|GetDA_Resource))) (Transformation|GetActorLocation) "0, 0, 0" 1.0 1.0 0.0 "/Game/Audio/NormalAttenuation.NormalAttenuation" 0 0 0)
    (Actor|DestroyActor)
    (return (Utilities|Struct|MakeApplyDamageOut true true))
    (else
      (return (Utilities|Struct|MakeApplyDamageOut true false)))))

(fn ClientInteractBP
  (params (InteractKey :type EInteractKey%20Enum :default "Interact1") (Pawn :type Pawn%20Object%20Reference) (BP_PAI :type BP%20PAI%20Object%20Reference))
  (return false))

(fn ClientInterruptBP
  (params (InterruptedBy :type EInterruptedBy%20Enum :default "Player") (InteractKey :type EInteractKey%20Enum :default "Interact1") (Pawn :type Pawn%20Object%20Reference) (BP_PAI :type BP%20PAI%20Object%20Reference))
  (return false))

(fn ServerInteractBP
  (params (InteractKey :type EInteractKey%20Enum :default "Interact1") (Pawn :type Pawn%20Object%20Reference) (BP_PAI :type BP%20PAI%20Object%20Reference))
  (for _array_element (Utilities|Struct|BreakResourceSize (Utilities|Array|Get(acopy) (Variables|/Script/SkyCraft.DA_Resource|GetSize (Variables|Default|GetDA_Resource))))
    (if (Math|Random|RandomBoolwithWeight (.Probability (Utilities|Struct|BreakResourceLoot _array_element)))
      (bind _inventory (Class|BPIGetInventory|GetInventory(Message) Pawn))
      (bind _success (Default|AddtoInventory _inventory (Utilities|Struct|MakeInventorySlot (.Item (Utilities|Struct|BreakResourceLoot _array_element)) (Math|Random|RandomIntegerinRange (.Min (Utilities|Struct|BreakResourceLoot _array_element)) (.Max (Utilities|Struct|BreakResourceLoot _array_element))))))
      (if _success
        (Actor|DestroyActor))))
  (return true))

(fn ServerInterruptBP
  (params (InterruptedBy :type EInterruptedBy%20Enum :default "Player") (InteractKey :type EInteractKey%20Enum :default "Interact1") (Pawn :type Pawn%20Object%20Reference) (BP_PAI :type BP%20PAI%20Object%20Reference))
  (return false))