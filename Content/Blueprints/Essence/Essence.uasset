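; Essence pickup actor whose color, derived from its Essence value, tints both its mesh material and Niagara effect.
; On the server, sphere overlap with a CharSpirit or PlayerIsland component passes the Essence to that actor and destroys the pickup.
; Spirit pickups also multicast a color-matched consume effect, attached to the consumer and skipped on dedicated servers.
; DestroyEssence removes it after a short random delay.
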(event OnComponentBeginOverlap(SphereCollision)
  (params (OverlappedComponent :type Primitive%20Component%20Object%20Reference) (OtherActor :type Actor%20Object%20Reference) (OtherComp :type Primitive%20Component%20Object%20Reference) (OtherBodyIndex :type Integer) (bFromSweep :type Boolean) (SweepResult :type Hit%20Result%20Structure%20%28by%20ref%29))
  (if (Networking|IsServer)
    (if (Components|ComponentHasTag OtherComp "CharSpirit")
      (Class|BPIEssence|ConsumeEssence(Message) OtherActor (Variables|Default|GetEssence))
      (CallFunction|MulticastNiagaraConsume OtherActor)
      (Actor|DestroyActor)
      (elif (Components|ComponentHasTag OtherComp "PlayerIsland")
        (Class|BPIEssence|ConsumeEssence(Message) OtherActor (Variables|Default|GetEssence))
        (Actor|DestroyActor)))))

(event Custom|Multicast_NiagaraConsume
  (params (ParentActor :type Actor%20Object%20Reference))
  (bind _essence (Variables|Default|GetEssence))
  (bind (_r _g _b) (CallFunction|EssenceRGB _essence))
  (if (not (Networking|IsDedicatedServer))
    (bind _returnvalue (Game|SpawnActorfromClass "/Game/Particles/a1Niagara.a1Niagara_C" (Math|Transform|MakeTransform "0, 0, 0" "0, 0, 0" "1.000000,1.000000,1.000000") "AlwaysSpawn" 0 "/Game/Particles/NS_Spirit_EssenceConsume.NS_Spirit_EssenceConsume" 0))
    (Transformation|AttachActorToActor _returnvalue ParentActor "None" "KeepRelative" "KeepRelative" "KeepRelative" true)
    (Niagara|SetNiagaraVariable(LinearColor) (Variables|/Game/Particles/a1Niagara.a1Niagara_C|GetNiagaraComponent _returnvalue) "EssenceColor" (Utilities|Struct|MakeLinearColor _r _g _b 1.0))))

(event Custom|DestroyEssence
  (Utilities|FlowControl|Delay (Math|Random|RandomFloatinRange 1.0 2.0))
  (Actor|DestroyActor))

(event EventBeginPlay
  (bind _essence (Variables|Default|GetEssence))
  (bind _essence_2 (Variables|Default|GetEssence))
  (bind (_r _g _b) (CallFunction|EssenceRGB _essence))
  (bind (_r_2 _g_2 _b_2) (CallFunction|EssenceRGB _essence_2))
  (bind _returnvalue (Rendering|Material|CreateDynamicMaterialInstance "/Game/GlobalMaterials/Essence/M_Essence.M_Essence" "None" "None" :!class /Script/Engine.KismetMaterialLibrary))
  (Rendering|Material|SetMaterial (Variables|Default|GetMesh) 0 _returnvalue)
  (Rendering|Material|SetVectorParameterValue _returnvalue "EssenceColor" (Utilities|Struct|MakeLinearColor _r_2 _g_2 _b_2 1.0) :!class /Script/Engine.MaterialInstanceDynamic)
  (Niagara|SetNiagaraVariable(LinearColor) (Variables|Default|GetNiagara) "EssenceColor" (Utilities|Struct|MakeLinearColor _r _g _b 1.0)))

(fn ConstructionScript)

(fn GetNiagara
  (return (Variables|Default|GetNiagara)))