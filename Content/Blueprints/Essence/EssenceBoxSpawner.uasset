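; Spawner actor that keeps a field of Essence actors around the followed player character.
; On BeginPlay it snaps to the character and spawns a set number of Essence at random points inside its box.
; Each tick it re-centers on the character and teleports any Essence outside the box to the opposite face, wrapping per axis so a fixed pool surrounds the moving player.
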(event EventTick
  (params (DeltaSeconds :type Float%20%28single-precision%29))
  (bind _box (Variables|Default|GetBox))
  (Utilities|IsValid (Variables|Default|GetFollowPlayerCharacter)
    (:Is%20Valid
      (Transformation|SetActorLocation (Transformation|GetActorLocation (Variables|Default|GetFollowPlayerCharacter)) false true)
      (for _array_element (Variables|Default|GetAllEssence)
        (Variables|Default|SetEachEssence _array_element)
        (if (not (Math|Geometry|IsPointinBox (Transformation|GetActorLocation (Variables|Default|GetEachEssence)) (Transformation|GetWorldLocation _box) (Components|Box|GetScaledBoxExtent _box)))
          (bind _newlocation (CallFunction|NewLocation (Transformation|GetActorLocation (Variables|Default|GetEachEssence))))
          (Transformation|SetActorLocation (Variables|Default|GetEachEssence) _newlocation false true))))))

(event EventBeginPlay
  (bind _box (Variables|Default|GetBox))
  (Transformation|SetActorLocation (Transformation|GetActorLocation (Variables|Default|GetFollowPlayerCharacter)) false true)
  (for _index (range 1 (Variables|Default|GetHowManyEssence))
    (bind _returnvalue (Game|SpawnActorfromClass :Class "/Game/Blueprints/Essence/Essence.Essence_C" :SpawnTransform (Math|Transform|MakeTransform (Math|Random|RandomPointinBoundingBox (Transformation|GetWorldLocation _box) (Components|Box|GetScaledBoxExtent _box)) "0, 0, 0" "1.000000,1.000000,1.000000") :CollisionHandlingOverride "AlwaysSpawn" :Instigator 0))
    (Utilities|Array|Add (Variables|Default|GetAllEssence) _returnvalue)))

(fn ConstructionScript)

(fn NewLocation
  (params (CurrentLocation :type Vector))
  (bind _box (Variables|Default|GetBox))
  (bind _returnvalue (Transformation|GetWorldLocation _box))
  (bind _returnvalue_2 (Components|Box|GetScaledBoxExtent _box))
  (LocalVariables|SetLocalX (.x CurrentLocation))
  (LocalVariables|SetLocalY (.y CurrentLocation))
  (LocalVariables|SetLocalZ (.z CurrentLocation))
  (LocalVariables|SetMaxX (+ (.x _returnvalue) (.x _returnvalue_2)))
  (LocalVariables|SetMinX (- (.x _returnvalue) (.x _returnvalue_2)))
  (LocalVariables|SetMaxY (+ (.y _returnvalue) (.y _returnvalue_2)))
  (LocalVariables|SetMinY (- (.y _returnvalue) (.y _returnvalue_2)))
  (LocalVariables|SetMaxZ (+ (.z _returnvalue) (.z _returnvalue_2)))
  (LocalVariables|SetMinZ (- (.z _returnvalue) (.z _returnvalue_2)))
  (Utilities|FlowControl|Sequence
    (:then_0
      (if (> (LocalVariables|GetLocalX) (LocalVariables|GetMaxX))
        (LocalVariables|SetLocalX (LocalVariables|GetMinX))))
    (:then_1
      (if (< (LocalVariables|GetLocalX) (LocalVariables|GetMinX))
        (LocalVariables|SetLocalX (LocalVariables|GetMaxX))))
    (:then_2
      (if (> (LocalVariables|GetLocalY) (LocalVariables|GetMaxY))
        (LocalVariables|SetLocalY (LocalVariables|GetMinY))))
    (:then_3
      (if (< (LocalVariables|GetLocalY) (LocalVariables|GetMinY))
        (LocalVariables|SetLocalY (LocalVariables|GetMaxY))))
    (:then_4
      (if (> (LocalVariables|GetLocalZ) (LocalVariables|GetMaxZ))
        (LocalVariables|SetLocalZ (LocalVariables|GetMinZ))))
    (:then_5
      (if (< (LocalVariables|GetLocalZ) (LocalVariables|GetMinZ))
        (LocalVariables|SetLocalZ (LocalVariables|GetMaxZ))))
    (:then_6
      (return (Math|Vector|MakeVector (LocalVariables|GetLocalX) (LocalVariables|GetLocalY) (LocalVariables|GetLocalZ))))))