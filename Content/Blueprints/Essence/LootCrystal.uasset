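; LootCrystal is an interactable loot actor holding Essence and an inventory, tinted by its essence color and destroyed once both are empty.
; Tapping it opens a loot widget suited to Normal or Spirit form, and Spirits can also drag it.
; Multicast drag events toggle collision, interaction and Tick, which trails the crystal behind the Spirit.
; On server overlap with a PlayerIsland component, a consumable crystal transfers its contents to that island.
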(event OnComponentBeginOverlap(StaticMesh)
  (params (OverlappedComponent :type Primitive%20Component%20Object%20Reference) (OtherActor :type Actor%20Object%20Reference) (OtherComp :type Primitive%20Component%20Object%20Reference) (OtherBodyIndex :type Integer) (bFromSweep :type Boolean) (SweepResult :type Hit%20Result%20Structure%20%28by%20ref%29))
  (if (Networking|IsServer)
    (if (Components|ComponentHasTag OtherComp "PlayerIsland")
      (if (Variables|Default|GetCanBeConsumedByPI?)
        (bind _islandarchon (Class|BPIIslandArchon|IslandArchon(Message) OtherActor))
        (Class|BPIEssence|ConsumeEssence(Message) _islandarchon (Variables|Default|GetEssence))
        (for _array_element (Variables|/Game/Blueprints/Inventory.Inventory_C|GetSlots (Variables|Default|GetAC_Inventory))
          (Default|AddtoInventory (Variables|/Game/Blueprints/IslandArchon.IslandArchon_C|GetInventory_Island _islandarchon) _array_element))
        (Actor|DestroyActor)))))

(event Custom|REMOVE_Inventory_Event_0
  (params (RemovedIndex :type Integer))
  (if (and (<= (Utilities|Array|Length (Variables|/Game/Blueprints/Inventory.Inventory_C|GetSlots (Variables|Default|GetAC_Inventory))) 0) (<= (CallFunction|EssenceTotal (Variables|Default|GetEssence)) 0))
    (Actor|DestroyActor)))

(event Custom|DestroyLootCrystal
  (Utilities|FlowControl|Delay (Math|Random|RandomFloatinRange 1.0 2.0))
  (Actor|DestroyActor))

(event Custom|EssenceChanged
  (if (and (<= (Utilities|Array|Length (Variables|/Game/Blueprints/Inventory.Inventory_C|GetSlots (Variables|Default|GetAC_Inventory))) 0) (<= (CallFunction|EssenceTotal (Variables|Default|GetEssence)) 0))
    (Actor|DestroyActor)))

(event Custom|OnDestroyed_Event_1
  (params (DestroyedActor :type Actor%20Object%20Reference))
  ;[0.6159 1 0.7401 1 125] Start Drag (Not Initial)
  (CallFunction|MulticastStopDrag)
  (Variables|Default|SetDrag_PF_Spirit 0) ; empty
)

(event EventSetDragChar
  (params (DragChar :type Actor%20Object%20Reference))
  (bind _aspf_spirit (Utilities|Casting|CastToPF_Spirit DragChar)
    (:then
      (Variables|Default|SetDrag_PF_Spirit _aspf_spirit))
    (:CastFailed
      (Variables|Default|SetDrag_PF_Spirit 0))))

(event EventTick
  (params (DeltaSeconds :type Float%20%28single-precision%29))
  (if (> (Transformation|GetDistanceTo (Variables|Default|GetDrag_PF_Spirit)) 7e+01)
    (Transformation|SetActorLocation (+ (Transformation|GetActorLocation (Variables|Default|GetDrag_PF_Spirit)) (* (Math|Vector|GetForwardVector (Math|Rotator|FindLookatRotation (Transformation|GetActorLocation (Variables|Default|GetDrag_PF_Spirit)) (Transformation|GetActorLocation))) 70)) false false)))

(event EventMulticastStartDrag
  ;[0.6159 1 0.7401 1 125] Start Drag (Not Initial)
  (Transformation|DetachFromActor "KeepWorld" "KeepWorld" "KeepWorld")
  (Collision|SetCollisionEnabled (Variables|Default|GetStaticMesh) "NoCollision")
  (Variables|/Game/Blueprints/InteractSystem/InteractSystem.InteractSystem_C|SetInteractable (Variables|Default|GetInteractSystem) false)
  (Actor|Tick|SetActorTickEnabled true)
  (if (Networking|IsServer)
    (Variables|Default|SetCanBeConsumedByPI? false)
    (Game|AssignOnDestroyed (Variables|Default|GetDrag_PF_Spirit) (delegate Custom|OnDestroyed_Event_1))))

(event EventMulticastStopDrag
  ;[1 0.4366 0.4665 1 125] Stop Drag
  (Utilities|IsValid (Variables|/Game/Blueprints/PF_Spirit.PF_Spirit_C|GetAttachedToIA (Variables|Default|GetDrag_PF_Spirit))
    (:Is%20Valid
      (Transformation|AttachActorToActor (Variables|/Game/Blueprints/PF_Spirit.PF_Spirit_C|GetAttachedToIA (Variables|Default|GetDrag_PF_Spirit)) "None" "KeepWorld" "KeepWorld" "KeepWorld" true))
    (:Is%20Not%20Valid
      _))
  (Collision|SetCollisionEnabled (Variables|Default|GetStaticMesh) "QueryAndPhysics")
  (Variables|/Game/Blueprints/InteractSystem/InteractSystem.InteractSystem_C|SetInteractable (Variables|Default|GetInteractSystem) true)
  (Actor|Tick|SetActorTickEnabled false)
  (Game|UnbindEventfromOnDestroyed (Variables|Default|GetDrag_PF_Spirit) (delegate Custom|OnDestroyed_Event_1)))

(event EventBeginPlay
  (CallFunction|UpdateColor)
  (EventDispatchers|AssignREMOVEInventory (Variables|Default|GetAC_Inventory) (delegate Custom|REMOVE_Inventory_Event_0))
  (EventDispatchers|BindEventtoEssenceChange (delegate Custom|EssenceChanged)))

(fn ConstructionScript)

(fn OnRepEssence
  (Default|CallEssenceChange)
  (CallFunction|UpdateColor))

(fn UpdateColor
  (bind _essence (Variables|Default|GetEssence))
  (bind _staticmesh (Variables|Default|GetStaticMesh))
  (bind (_r _g _b) (CallFunction|EssenceRGB _essence))
  (Utilities|IsValid _staticmesh
    (:Is%20Valid
      (Rendering|Material|SetVectorParameterValueonMaterials _staticmesh "EssenceColor" (Math|Vector|MakeVector _r _g _b)))))

(fn ClientInterrupt
  (params (InterruptedBy :type E_InterruptedBy%20Enum :default "NewEnumerator0") (InteractKey :type E_InteractKey%20Enum :default "NewEnumerator0") (InteractedPawn :type Pawn%20Object%20Reference) (InteractedPC_Sky :type PC%20Sky%20Object%20Reference) (InteractedPP_Sky :type PP%20Sky%20Object%20Reference))
  (return false))

(fn ClientTapInteract
  (params (InteractedKey :type E_InteractKey%20Enum :default "NewEnumerator0") (InteractedPawn :type Pawn%20Object%20Reference) (InteractedPC_Sky :type PC%20Sky%20Object%20Reference) (InteractedPP_Sky :type PP%20Sky%20Object%20Reference) (InteractedWith :type IC%20Class%20Reference))
  (switch Utilities|FlowControl|Switch|SwitchonE_PlayerForm (Variables|/Game/Blueprints/PP_Sky.PP_Sky_C|GetCurrentPlayerForm InteractedPP_Sky)
    (:NewEnumerator2
      (if (> (Utilities|Array|Length (Variables|/Game/Blueprints/Inventory.Inventory_C|GetSlots (Variables|Default|GetAC_Inventory))) 1)
        (bind _returnvalue (UserInterface|CreateWidget "/Game/Widgets/CWS/CWS_LootCrystal_Normal.CWS_LootCrystal_Normal_C" InteractedPC_Sky self (Variables|Default|GetAC_Inventory) 0 InteractedPC_Sky InteractedPawn))
        (UserInterface|Viewport|AddtoViewport _returnvalue 0)
        (Default|AddCWS InteractedPC_Sky _returnvalue true true "NewEnumerator2")))
    (:NewEnumerator3
      (bind _returnvalue_2 (UserInterface|CreateWidget "/Game/Widgets/CWS/CWS_LootCrystal_Spirit.CWS_LootCrystal_Spirit_C" InteractedPC_Sky InteractedPC_Sky self (Variables|Default|GetAC_Inventory) 0 InteractedPC_Sky InteractedPawn))
      (UserInterface|Viewport|AddtoViewport _returnvalue_2 0)
      (Default|AddCWS InteractedPC_Sky _returnvalue_2 true true "NewEnumerator2")
      (return true))))

(fn ConsumeEssence
  (params (Essence :type S%20Essence%20Structure))
  (return false))

(fn GetInteractLocation
  (return (Transformation|GetActorLocation)))

(fn GetInteractSystem
  (return (Variables|Default|GetInteractSystem)))

(fn GetEssence
  (return ""))

(fn ServerInterrupt
  (params (InterruptedBy :type E_InterruptedBy%20Enum :default "NewEnumerator0") (InteractKey :type E_InteractKey%20Enum :default "NewEnumerator0") (InteractedPawn :type Pawn%20Object%20Reference) (InteractedPC_Sky :type PC%20Sky%20Object%20Reference) (InteractedPP_Sky :type PP%20Sky%20Object%20Reference))
  (return false))

(fn ServerTapInteract
  (params (InteractedKey :type E_InteractKey%20Enum :default "NewEnumerator0") (InteractedPawn :type Pawn%20Object%20Reference) (InteractedPC_Sky :type PC%20Sky%20Object%20Reference) (InteractedPP_Sky :type PP%20Sky%20Object%20Reference) (InteractedWith :type IC%20Class%20Reference))
  (switch Utilities|FlowControl|Switch|SwitchonE_InteractKey InteractedKey
    (:NewEnumerator2
      (switch Utilities|FlowControl|Switch|SwitchonE_PlayerForm (Variables|/Game/Blueprints/PP_Sky.PP_Sky_C|GetCurrentPlayerForm InteractedPP_Sky)
        (:NewEnumerator2
          (return false))
        (:NewEnumerator3
          (Default|ServerStartDrag (Variables|/Game/Blueprints/PF_Normal.PF_Normal_C|GetPF_Spirit (Variables|/Game/Blueprints/PP_Sky.PP_Sky_C|GetPF_Normal InteractedPP_Sky)) self)
          (return true))))))

(fn SetEssence(Server)
  (params (Essence :type S%20Essence%20Structure))
  (bind _output_get (Variables|Default|SetEssence Essence))
  (return _output_get))