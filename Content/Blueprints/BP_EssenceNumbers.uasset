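; Short-lived actor that shows a "+N" essence number through a widget component.
; On BeginPlay it fills the W_EssenceNumbers text with the total of its Essence value and colors it from that essence's RGB conversion.
; It rebuilds the font info so the outline takes the same color at half opacity.
; It binds to the widget's finished-animation event and destroys itself when that fires.
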(event Custom|FinishedAnimation
  (Actor|DestroyActor))

(event EventBeginPlay
  (bind _essence (Variables|Default|GetEssence))
  (bind _returnvalue (Class|AdianFL|EssencetoRGB _essence))
  (bind _asw_essence_numbers (Utilities|Casting|CastToW_EssenceNumbers (UserInterface|GetWidget (Variables|Default|GetWidgetComponent))))
  (bind _output_get (Variables|Default|SetW_EssenceNumbers _asw_essence_numbers))
  (bind _output_get_2 (Variables|Default|SetText (Variables|/Game/Widgets/W_EssenceNumbers.W_EssenceNumbers_C|GetText _output_get)))
  (Rendering|Components|TextRender|SetText _output_get_2 (Utilities|Text|FormatText "+{0}" (Utilities|Text|ToText(Integer) (Class|AdianFL|EssenceTotal (Variables|Default|GetEssence)))))
  (Appearance|SetColorandOpacity (Variables|Default|GetText) (Utilities|Struct|MakeSlateColor (Class|AdianFL|EssencetoRGB (Variables|Default|GetEssence)) "UseColor_Specified") :!class /Script/UMG.TextBlock)
  (bind _structout (Utilities|Struct|SetmembersinSlateFontInfo (Utilities|Struct|MakeSlateFontInfo (.FontObject (Utilities|Struct|BreakSlateFontInfo (Variables|/Script/UMG.TextBlock|GetFont (Variables|Default|GetText)))) (.FontMaterial (Utilities|Struct|BreakSlateFontInfo (Variables|/Script/UMG.TextBlock|GetFont (Variables|Default|GetText)))) (Utilities|Struct|MakeFontOutlineSettings (.OutlineSize (Utilities|Struct|BreakFontOutlineSettings (.OutlineSettings (Utilities|Struct|BreakSlateFontInfo (Variables|/Script/UMG.TextBlock|GetFont (Variables|Default|GetText)))))) false (.bSeparateFillAlpha (Utilities|Struct|BreakFontOutlineSettings (.OutlineSettings (Utilities|Struct|BreakSlateFontInfo (Variables|/Script/UMG.TextBlock|GetFont (Variables|Default|GetText)))))) (.bApplyOutlineToDropShadows (Utilities|Struct|BreakFontOutlineSettings (.OutlineSettings (Utilities|Struct|BreakSlateFontInfo (Variables|/Script/UMG.TextBlock|GetFont (Variables|Default|GetText)))))) (.OutlineMaterial (Utilities|Struct|BreakFontOutlineSettings (.OutlineSettings (Utilities|Struct|BreakSlateFontInfo (Variables|/Script/UMG.TextBlock|GetFont (Variables|Default|GetText)))))) (Utilities|Struct|MakeLinearColor (.r _returnvalue) (.g _returnvalue) (.b _returnvalue) 0.5)) (.TypefaceFontName (Utilities|Struct|BreakSlateFontInfo (Variables|/Script/UMG.TextBlock|GetFont (Variables|Default|GetText)))) (.Size (Utilities|Struct|BreakSlateFontInfo (Variables|/Script/UMG.TextBlock|GetFont (Variables|Default|GetText)))) (.LetterSpacing (Utilities|Struct|BreakSlateFontInfo (Variables|/Script/UMG.TextBlock|GetFont (Variables|Default|GetText)))))))
  (Class|TextBlock|SetFont (Variables|Default|GetText) _structout)
  (EventDispatchers|BindEventtoFinishedAnimation (Variables|Default|GetW_EssenceNumbers) (delegate Custom|FinishedAnimation)))

(fn ConstructionScript)