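; Player island component that burns the island Archon's selected red, green and blue Essence to pay for travel speed above 1.
; Each tick removes one unit per selected colour, deselecting any that is empty.
; On stop-state changes (bound on the server) or depletion, it sets tick interval to selected count over excess speed, making tick rate the burn rate.
; Ticking halts when stopped or not boosted; having no selection also resets target speed to 1.
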(event Custom|StopIslandChanged
  (CallFunction|UpdateTickBurnMatch))

(event EventBeginPlay
  (if (Networking|IsServer)
    (bind _islandarchon (Class|BPIIslandArchon|IslandArchon(Message) (Components|GetOwner)))
    (bind _output_get (Variables|Default|SetIslandArchon _islandarchon))
    (EventDispatchers|BindEventtoStopIslandChange _output_get (delegate Custom|StopIslandChanged))))

(event EventTick
  (params (DeltaSeconds :type Float%20%28single-precision%29))
  (bind _islandarchon (Variables|Default|GetIslandArchon))
  (bind _islandarchon_2 (Variables|Default|GetIslandArchon))
  (bind _islandarchon_3 (Variables|Default|GetIslandArchon))
  (Utilities|FlowControl|Sequence
    (:then_0
      (Variables|Default|SetTempEssence (Variables|/Game/Blueprints/IslandArchon.IslandArchon_C|GetEssence (Variables|Default|GetIslandArchon)))
      (Utilities|FlowControl|Sequence
        (:then_0
          (if (.red (Variables|/Game/Blueprints/IslandArchon.IslandArchon_C|GetEssenceBurnSelect (Variables|Default|GetIslandArchon))) ; Burn Red Slected?
            (if (> (.red (Variables|Default|GetTempEssence)) 0) ; Red > 0
              (Variables|Default|SetTempEssence (Utilities|Struct|MakeS_Essence (- (.red (Variables|Default|GetTempEssence)) 1) (.green (Variables|Default|GetTempEssence)) (.blue (Variables|Default|GetTempEssence)))) ; Burn 1 Red
            )
            (if (not (> (.red (Variables|Default|GetTempEssence)) 0)) ; Red > 0
              (Variables|/Game/Blueprints/IslandArchon.IslandArchon_C|SetEssenceBurnSelect _islandarchon (Utilities|Struct|MakeS_EssenceSelect false (.green (Variables|/Game/Blueprints/IslandArchon.IslandArchon_C|GetEssenceBurnSelect _islandarchon)) (.blue (Variables|/Game/Blueprints/IslandArchon.IslandArchon_C|GetEssenceBurnSelect _islandarchon)))) ; Disable Red
              (CallFunction|UpdateTickBurnMatch))))
        (:then_1
          (if (.green (Variables|/Game/Blueprints/IslandArchon.IslandArchon_C|GetEssenceBurnSelect (Variables|Default|GetIslandArchon)))
            (if (> (.green (Variables|Default|GetTempEssence)) 0) ; Green > 0
              (Variables|Default|SetTempEssence (Utilities|Struct|MakeS_Essence (.red (Variables|Default|GetTempEssence)) (- (.green (Variables|Default|GetTempEssence)) 1) (.blue (Variables|Default|GetTempEssence)))) ; Burn 1 Green
            )
            (if (not (> (.green (Variables|Default|GetTempEssence)) 0)) ; Green > 0
              (Variables|/Game/Blueprints/IslandArchon.IslandArchon_C|SetEssenceBurnSelect _islandarchon_2 (Utilities|Struct|MakeS_EssenceSelect (.red (Variables|/Game/Blueprints/IslandArchon.IslandArchon_C|GetEssenceBurnSelect _islandarchon_2)) false (.blue (Variables|/Game/Blueprints/IslandArchon.IslandArchon_C|GetEssenceBurnSelect _islandarchon_2)))) ; Disable Green
              (CallFunction|UpdateTickBurnMatch))))
        (:then_2
          (if (.blue (Variables|/Game/Blueprints/IslandArchon.IslandArchon_C|GetEssenceBurnSelect (Variables|Default|GetIslandArchon)))
            (if (> (.blue (Variables|Default|GetTempEssence)) 0) ; Blue > 0
              (Variables|Default|SetTempEssence (Utilities|Struct|MakeS_Essence (.red (Variables|Default|GetTempEssence)) (.green (Variables|Default|GetTempEssence)) (- (.blue (Variables|Default|GetTempEssence)) 1))) ; Burn 1 Blue
            )
            (if (not (> (.blue (Variables|Default|GetTempEssence)) 0)) ; Blue > 0
              (Variables|/Game/Blueprints/IslandArchon.IslandArchon_C|SetEssenceBurnSelect _islandarchon_3 (Utilities|Struct|MakeS_EssenceSelect (.red (Variables|/Game/Blueprints/IslandArchon.IslandArchon_C|GetEssenceBurnSelect _islandarchon_3)) (.green (Variables|/Game/Blueprints/IslandArchon.IslandArchon_C|GetEssenceBurnSelect _islandarchon_3)) false)) ; Diisable Blue
              (CallFunction|UpdateTickBurnMatch))))))
    (:then_1
      (Variables|/Game/Blueprints/IslandArchon.IslandArchon_C|SetEssence (Variables|Default|GetIslandArchon) (Variables|Default|GetTempEssence)))))

(fn UpdateTickBurnMatch
  (bind _islandarchon (Variables|Default|GetIslandArchon))
  (bind _essenceburnselect (Variables|/Game/Blueprints/IslandArchon.IslandArchon_C|GetEssenceBurnSelect _islandarchon))
  (if (Variables|/Game/Blueprints/IslandArchon.IslandArchon_C|GetStopIsland (Variables|Default|GetIslandArchon))
    (Components|Tick|SetComponentTickEnabled false)
    (elif (> (Variables|/Game/Blueprints/IslandArchon.IslandArchon_C|GetTargetSpeed (Variables|Default|GetIslandArchon)) 1.0)
      (Utilities|FlowControl|Sequence
        (:then_0
          (if (.red _essenceburnselect)
            (LocalVariables|SetEssenceSelectNum (+ 1 (LocalVariables|GetEssenceSelectNum)) :!label _label)))
        (:then_1
          (if (.green _essenceburnselect)
            (goto _label)))
        (:then_2
          (if (.blue _essenceburnselect)
            (goto _label)))
        (:then_3
          (if (> (LocalVariables|GetEssenceSelectNum) 0)
            (Class|ActorComponent|SetComponentTickInterval (/ (LocalVariables|GetEssenceSelectNum) (- (Variables|/Game/Blueprints/IslandArchon.IslandArchon_C|GetTargetSpeed (Variables|Default|GetIslandArchon)) 1.0)))
            (Components|Tick|SetComponentTickEnabled true)
            (else
              (Variables|/Game/Blueprints/IslandArchon.IslandArchon_C|SetTargetSpeed (Variables|Default|GetIslandArchon) 1.0)
              (Components|Tick|SetComponentTickEnabled false)))))
      (else
        (Components|Tick|SetComponentTickEnabled false)))))