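; PawnTempCamera is a temporary camera actor, owned by a BP_PCS, that can serve as that owner's view target.
; On BeginPlay it caches the owner, attaches to an optional parent keeping world location, and, on the server, optionally blends the view to itself.
; A client-ready event relays to the server, whose ready event triggers CallClientCameraReady, then destroys the actor after a configurable delay.
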(event Custom|Server_Ready
  (Default|CallClientCameraReady)
  (Utilities|FlowControl|Delay (Variables|Default|GetDestroyTime))
  (Actor|DestroyActor))

(event Custom|Client_Ready
  (CallFunction|ServerReady))

(event EventBeginPlay
  (bind _asbp_pcs (Utilities|Casting|CastToBP_PCS (Components|GetOwner))
    (:then
      _)
    (:CastFailed
      _))
  (Variables|Default|SetBP_PCS _asbp_pcs)
  (bind _attachparent (Variables|Default|GetAttachParent)
    (:then
      (Transformation|AttachActorToActor _attachparent "None" "KeepWorld" "KeepRelative" "KeepRelative" true))
    (:else
      _))
  (if (Networking|IsServer)
    (if (Variables|Default|GetSetViewTarget)
      (Game|Player|SetViewTargetwithBlend (Variables|Default|GetBP_PCS) self 0.0 "VTBlend_Linear" 0.0 false))))

(fn ConstructionScript)