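; Island chunk actor that removes itself and its spawned Island once its HMPR counter drops to zero or below.
; The HMPR RepNotify triggers DestroyChunk.
; DestroyChunk uses the chunk's index in GMSky's SpawnedChunkIslands to clear both that array and the parallel SpawnedChunkIslandsCors, then destroys the Island if valid and the chunk itself.
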(fn ConstructionScript)

(fn DestroyChunk
  (bind _self self)
  (bind _island (Variables|Default|GetIsland))
  (bind _gm_sky (Variables|Default|GetGM_Sky))
  (bind _gm_sky_2 (Variables|Default|GetGM_Sky))
  (bind _spawnedchunkislands (Variables|/Game/Blueprints/GM_Sky.GM_Sky_C|GetSpawnedChunkIslands _gm_sky_2))
  (bind _returnvalue (Utilities|Array|FindItem _spawnedchunkislands _self))
  (Utilities|Array|RemoveIndex (Variables|/Game/Blueprints/GM_Sky.GM_Sky_C|GetSpawnedChunkIslandsCors _gm_sky) _returnvalue)
  (Utilities|Array|RemoveIndex (Variables|/Game/Blueprints/GM_Sky.GM_Sky_C|GetSpawnedChunkIslands _gm_sky) _returnvalue)
  (Utilities|IsValid _island
    (:Is%20Valid
      (Actor|DestroyActor _island))
    (:Is%20Not%20Valid
      _))
  (Actor|DestroyActor))

(fn OnRepHMPR
  (if (<= (Variables|Default|GetHMPR) 0)
    (CallFunction|DestroyChunk)))