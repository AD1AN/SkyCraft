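; Main menu island: a voxel world that builds itself at BeginPlay with a seed from IslandSeeds (random if empty) and a random scale within IslandScale.
; Once the world loads, it waits briefly, has BPResourceGenerator scatter KarkTree resources within a slope limit, then calls Loaded.
; UpdateVoxels increments the first stored seed, picks a seed again and rebuilds the world.
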(event Custom|OnWroldLoaded
  (Utilities|FlowControl|Delay 0.5)
  (Class|ResourceGenerator|GenerateResources (Variables|Default|GetBP_ResourceGenerator) (Utilities|Struct|MakeGenerateResourcesIn 2000 "/Game/DataAssets/Resource/KarkTree.KarkTree" 35.0 (Utilities|Struct|MakeUint8MinMax 2 3) "(Min=0,Max=0)"))
  (Default|CallLoaded))

(event EventBeginPlay
  (bind _islandscale (Variables|Default|GetIslandScale))
  (bind _islandseeds (Variables|Default|GetIslandSeeds))
  (bind _generator (Variables|Default|GetGenerator))
  (if (not (Class|VoxelWorld|IsCreated))
    (Class|VoxelGeneratorTools|SetGeneratorParameter _generator "SeedName" (Math|Integer|SelectInt (Math|Random|RandomInteger 21474836) (.OutItem (Utilities|Array|Random _islandseeds)) (== (Utilities|Array|Length _islandseeds) 0)))
    (Class|VoxelGeneratorTools|SetGeneratorParameter _generator "Scale" (Math|Random|RandomIntegerinRange (Math|Float|Truncate (.x _islandscale)) (Math|Float|Truncate (.y _islandscale))))
    (Class|VoxelWorld|CreateWorld)
    (Default|SetupGenerator (Variables|Default|GetBP_ResourceGenerator) (Utilities|Struct|MakeSetupGeneratorIn 1e+05 (Math|Random|RandomInteger 15) 1.0 4e+04 -5e+04))
    (EventDispatchers|AssignOnWorldLoaded (delegate Custom|OnWroldLoaded))))

(fn ConstructionScript)

(fn UpdateVoxels
  (bind _islandseeds (Variables|Default|GetIslandSeeds))
  (Utilities|Array|SetArrayElem (Variables|Default|GetIslandSeeds) 0 (+ (Utilities|Array|Get(acopy) _islandseeds) 1))
  (Class|VoxelGeneratorTools|SetGeneratorParameter (Variables|Default|GetGenerator) "SeedName" (Math|Integer|SelectInt (Math|Random|RandomInteger 21474836) (.OutItem (Utilities|Array|Random _islandseeds)) (== (Utilities|Array|Length _islandseeds) 0)))
  (Class|VoxelWorld|DestroyWorld)
  (Class|VoxelWorld|CreateWorld))