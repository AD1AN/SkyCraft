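; Main menu character that previews the currently selected character's bio.
; The construction script slaves chest, legs, feet, head and hand meshes to the main Mesh through master pose.
; BeginPlay caches the anim instance and binds to the selected-character change in the game instance's custom settings.
; Each change reapplies the bio, swapping the male or female body mesh and setting hair color, eye color and skin tone material parameters.
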(event Custom|SelectedCharacter_Changed_Event_0
  (params (Index :type Integer))
  (CallFunction|ApplyCharacterBio (Default|GetSelectedCharacterBio (Variables|/Game/Blueprints/SGI.SGI_C|GetCustomSettings (Variables|Default|GetSGI)))))

(event EventBeginPlay
  (bind _asab_main_menu (Utilities|Casting|CastToAB_MainMenu (Components|SkeletalMesh|GetAnimInstance (Variables|Character|GetMesh))))
  (Variables|Default|SetAnimBP _asab_main_menu)
  (bind _sgi (Class|BPISGI|GetSGI(Message) (Game|GetGameInstance)))
  (bind _output_get (Variables|Default|SetSGI _sgi))
  (EventDispatchers|AssignSelectedCharacterChanged (Variables|/Game/Blueprints/SGI.SGI_C|GetCustomSettings _output_get) (delegate Custom|SelectedCharacter_Changed_Event_0)))

(fn ConstructionScript
  (Class|SkinnedMeshComponent|SetMasterPoseComponent (Variables|Default|GetSM_Chest) (Variables|Character|GetMesh) false))

(fn ApplyCharacterBio
  (params (S_CharacterBio :type S%20Character%20Bio%20Structure))
  (bind _haircolor (Utilities|Struct|BreakS_CharacterBio S_CharacterBio))
  (bind _eyecolor (Utilities|Struct|BreakS_CharacterBio S_CharacterBio))
  (bind (_r _g _b) (Utilities|Struct|BreakLinearColor _eyecolor))
  (bind (_r_2 _g_2 _b_2) (Utilities|Struct|BreakLinearColor _haircolor))
  (Class|SkinnedMeshComponent|SetSkeletalMesh (Variables|Character|GetMesh) (select (.Gender (Utilities|Struct|BreakS_CharacterBio S_CharacterBio)) "/Game/Characters/Male/Male.Male" "/Game/Characters/Female/Female.Female") false)
  (Rendering|Material|SetVectorParameterValueonMaterials (Variables|Default|GetHair1) "HairColor" (Math|Vector|MakeVector _r_2 _g_2 _b_2))
  (Rendering|Material|SetVectorParameterValueonMaterials (Variables|Character|GetMesh) "EyeColor" (Math|Vector|MakeVector _r _g _b))
  (Rendering|Material|SetScalarParameterValueonMaterials (Variables|Character|GetMesh) "SkinTone" (.SkinTone (Utilities|Struct|BreakS_CharacterBio S_CharacterBio)))
  (return true))