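; Interactable loot crystal that holds an inventory and replicated Essence, tints its material by Essence, and destroys itself when both are empty.
; Interaction opens form-specific loot widgets, and Spirit players can drag it, with Tick keeping it leashed behind the spirit.
; Dragging disables collision and interaction until stopped or the spirit is destroyed.
; On server overlap, a consumable crystal gives its contents to the Island Archon and is destroyed.
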(event OnComponentBeginOverlap(StaticMesh)
  (params (OverlappedComponent :type Primitive%20Component%20Object%20Reference) (OtherActor :type Actor%20Object%20Reference) (OtherComp :type Primitive%20Component%20Object%20Reference) (OtherBodyIndex :type Integer) (bFromSweep :type Boolean) (SweepResult :type Hit%20Result%20Structure%20%28by%20ref%29))
  (if (Networking|IsServer)
    (if (Variables|Default|GetCanBeConsumedByIA?)
      (bind _asbp_island_archon (Utilities|Casting|CastToBP_IslandArchon OtherActor))
      (Class|EssenceInterface|AddEssence(Message) _asbp_island_archon (Variables|Default|GetEssence))
      (for _array_element (Variables|/Script/SkyCraft.Inventory|GetSlots (Variables|Default|GetInventory))
        (Class|Inventory|InsertSlot (Variables|/Game/Blueprints/BP_IslandArchon.BP_IslandArchon_C|GetInventory _asbp_island_archon) _array_element))
      (Actor|DestroyActor))))

(event Custom|REMOVE_Inventory_Event_0
  (params (RemovedIndex :type Integer))
  (if (and (<= (Utilities|Array|Length (Variables|/Script/SkyCraft.Inventory|GetSlots (Variables|Default|GetInventory))) 0) (<= (Class|AdianFL|EssenceTotal (Variables|Default|GetEssence)) 0))
    (Actor|DestroyActor)))

(event Custom|DestroyLootCrystal
  (Utilities|FlowControl|Delay (Math|Random|RandomFloatinRange 1.0 2.0))
  (Actor|DestroyActor))

(event Custom|EssenceChanged
  (if (and (<= (Utilities|Array|Length (Variables|/Script/SkyCraft.Inventory|GetSlots (Variables|Default|GetInventory))) 0) (<= (Class|AdianFL|EssenceTotal (Variables|Default|GetEssence)) 0))
    (Actor|DestroyActor)))

(event Custom|OnDestroyed_Event_1
  (params (DestroyedActor :type Actor%20Object%20Reference))
  ;[0.6159 1 0.7401 1 125] Start Drag (Not Initial)
  (CallFunction|MulticastStopDrag)
  (Variables|Default|SetDrag_PF_Spirit 0) ; empty
)

(event EventSetDragChar
  (params (DragChar :type Actor%20Object%20Reference))
  (bind _aspf_spirit (Utilities|Casting|CastToPF_Spirit DragChar)
    (:then
      (Variables|Default|SetDrag_PF_Spirit _aspf_spirit))
    (:CastFailed
      (Variables|Default|SetDrag_PF_Spirit 0))))

(event EventTick
  (params (DeltaSeconds :type Float%20%28single-precision%29))
  (if (> (Transformation|GetDistanceTo (Variables|Default|GetDrag_PF_Spirit)) 7e+01)
    (Transformation|SetActorLocation (+ (Transformation|GetActorLocation (Variables|Default|GetDrag_PF_Spirit)) (* (Math|Vector|GetForwardVector (Math|Rotator|FindLookatRotation (Transformation|GetActorLocation (Variables|Default|GetDrag_PF_Spirit)) (Transformation|GetActorLocation))) 70)) false false)))

(event EventMulticastStartDrag
  ;[0.6159 1 0.7401 1 125] Start Drag (Not Initial)
  (Transformation|DetachFromActor "KeepWorld" "KeepWorld" "KeepWorld")
  (Collision|SetCollisionEnabled (Variables|Default|GetStaticMesh) "NoCollision")
  (Class|InteractSystem|SetInteractable (Variables|Default|GetInteractSystem) false)
  (Actor|Tick|SetActorTickEnabled true)
  (if (Networking|IsServer)
    (Variables|Default|SetCanBeConsumedByIA? false)
    (Game|AssignOnDestroyed (Variables|Default|GetDrag_PF_Spirit) (delegate Custom|OnDestroyed_Event_1))))

(event EventMulticastStopDrag
  ;[1 0.4366 0.4665 1 125] Stop Drag
  (Utilities|IsValid (Variables|/Game/Blueprints/PF_Spirit.PF_Spirit_C|GetAttachedToIA (Variables|Default|GetDrag_PF_Spirit))
    (:Is%20Valid
      (Transformation|AttachActorToActor (Variables|/Game/Blueprints/PF_Spirit.PF_Spirit_C|GetAttachedToIA (Variables|Default|GetDrag_PF_Spirit)) "None" "KeepWorld" "KeepWorld" "KeepWorld" true))
    (:Is%20Not%20Valid
      _))
  (Collision|SetCollisionEnabled (Variables|Default|GetStaticMesh) "QueryAndPhysics")
  (Class|InteractSystem|SetInteractable (Variables|Default|GetInteractSystem) true)
  (Actor|Tick|SetActorTickEnabled false)
  (Game|UnbindEventfromOnDestroyed (Variables|Default|GetDrag_PF_Spirit) (delegate Custom|OnDestroyed_Event_1)))

(event EventBeginPlay
  (CallFunction|UpdateColor)
  (EventDispatchers|BindEventtoEssenceChange (delegate Custom|EssenceChanged)))

(fn ConstructionScript)

(fn OnRepEssence
  (Default|CallEssenceChange)
  (CallFunction|UpdateColor))

(fn UpdateColor
  (bind _essence (Variables|Default|GetEssence))
  (bind _staticmesh (Variables|Default|GetStaticMesh))
  (bind _returnvalue (Class|AdianFL|EssencetoRGB _essence))
  (Utilities|IsValid _staticmesh
    (:Is%20Valid
      (Rendering|Material|SetVectorParameterValueonMaterials _staticmesh "EssenceColor" (Math|Vector|MakeVector (.r _returnvalue) (.g _returnvalue) (.b _returnvalue))))))

(fn ClientInteractBP
  (params (InteractKey :type EInteractKey%20Enum :default "Interact1") (Pawn :type Pawn%20Object%20Reference) (BP_PSS :type BP%20PSS%20Object%20Reference))
  (switch Utilities|FlowControl|Switch|SwitchonEPlayerForm (Variables|/Script/SkyCraft.PSS|GetPlayerForm BP_PSS)
    (:Normal
      (if (> (Utilities|Array|Length (Variables|/Script/SkyCraft.Inventory|GetSlots (Variables|Default|GetInventory))) 1)
        (bind _returnvalue (UserInterface|CreateWidget "/Game/Widgets/CWS/CWS_LootCrystal_Normal.CWS_LootCrystal_Normal_C" 0 self (Variables|Default|GetInventory)))
        (UserInterface|Viewport|AddtoViewport _returnvalue 0)
        (Default|AddCWS BP_PSS _returnvalue true true true "NewEnumerator2")))
    (:Spirit
      (bind _returnvalue_2 (UserInterface|CreateWidget "/Game/Widgets/CWS/CWS_LootCrystal_Spirit.CWS_LootCrystal_Spirit_C" 0 self (Variables|Default|GetInventory)))
      (UserInterface|Viewport|AddtoViewport _returnvalue_2 0)
      (Default|AddCWS BP_PSS _returnvalue_2 true true true "NewEnumerator2")
      (return true))))

(fn ClientInterruptBP
  (params (InterruptedBy :type EInterruptedBy%20Enum :default "Player") (InteractKey :type EInteractKey%20Enum :default "Interact1") (Pawn :type Pawn%20Object%20Reference) (BP_PSS :type BP%20PSS%20Object%20Reference))
  (return false))

(fn ServerInteractBP
  (params (InteractKey :type EInteractKey%20Enum :default "Interact1") (Pawn :type Pawn%20Object%20Reference) (BP_PSS :type BP%20PSS%20Object%20Reference))
  (switch Utilities|FlowControl|Switch|SwitchonEInteractKey InteractKey
    (:Interact3
      (switch Utilities|FlowControl|Switch|SwitchonEPlayerForm (Variables|/Script/SkyCraft.PSS|GetPlayerForm BP_PSS)
        (:Normal
          (return false))
        (:Spirit
          (Default|ServerStartDrag (Variables|/Game/Blueprints/PF_Normal.PF_Normal_C|GetPF_Spirit (Variables|/Game/Blueprints/BP_PSS.BP_PSS_C|GetPF_Normal BP_PSS)) self)
          (return false))))))

(fn ServerInterruptBP
  (params (InterruptedBy :type EInterruptedBy%20Enum :default "Player") (InteractKey :type EInteractKey%20Enum :default "Interact1") (Pawn :type Pawn%20Object%20Reference) (BP_PSS :type BP%20PSS%20Object%20Reference))
  (return false))