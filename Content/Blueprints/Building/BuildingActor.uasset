(event EventBeginPlay
  (for _array_element (Actor|GetComponentsByClass "/Script/Engine.StaticMeshComponent")
    (Utilities|Array|Add (Variables|Default|GetBuildingMaterials) (Rendering|Material|GetMaterial _array_element 0))))

(fn ConstructionScript)

(fn PreviewMode
  (params (PreviewMode :type Boolean))
  (bind _returnvalue (Actor|GetComponentsByClass "/Script/Engine.StaticMeshComponent"))
  (if PreviewMode
    (for _array_element _returnvalue
      (Rendering|Material|SetMaterial _array_element 0 "/Game/GlobalMaterials/M_BuildingPreview.M_BuildingPreview"))
    (else
      (for (_array_element_2 _array_index) _returnvalue
        (Rendering|Material|SetMaterial _array_element_2 0 (Utilities|Array|Get(acopy) (Variables|Default|GetBuildingMaterials) _array_index))))))

(fn CollisionMode
  (params (CollisionMode :type ECollisionEnabled%20Enum :default "NoCollision"))
  (bind _returnvalue (Utilities|Select :Index CollisionMode :NoCollision false :QueryOnly false :PhysicsOnly true :QueryAndPhysics true))
  (Utilities|FlowControl|Sequence
    (:then_0
      (Collision|SetActorEnableCollision _returnvalue))
    (:then_1
      (for _array_element (Actor|GetAllChildActors false)
        (Collision|SetActorEnableCollision _array_element _returnvalue)))))

(fn EditRotation
  (params (Up :type Boolean))
  (bind _returnvalue (Transformation|GetActorRotation))
  (bind _returnvalue_2 (Transformation|GetActorRotation))
  (if Up
    (Transformation|SetActorRotation (Math|Rotator|MakeRotator (.roll _returnvalue_2) (.pitch _returnvalue_2) (+ (.yaw _returnvalue_2) (Variables|Default|GetBuildingRotation))))
    (else
      (Transformation|SetActorRotation (Math|Rotator|MakeRotator (.roll _returnvalue) (.pitch _returnvalue) (- (.yaw _returnvalue) (Variables|Default|GetBuildingRotation)))))))

(fn ApplyEdit
  (bind _ac_interact (Variables|Default|GetAC_Interact))
  (Variables|/Game/Blueprints/AC_Interact.AC_Interact_C|SetP_Edit_Pawn _ac_interact 0)
  (Components|Tick|SetComponentTickEnabled _ac_interact false)
  (Modes|PreviewMode false)
  (Widget|RemovefromParent (Variables|Default|GetW_EditMode))
  (Variables|Default|SetW_EditMode 0))

(fn DiscardEdit
  (bind _returnvalue (Transformation|GetActorRotation))
  (bind _ac_interact (Variables|Default|GetAC_Interact))
  (Variables|/Game/Blueprints/AC_Interact.AC_Interact_C|SetP_Edit_Pawn _ac_interact 0)
  (Components|Tick|SetComponentTickEnabled _ac_interact false)
  (Transformation|SetActorRotation (Math|Rotator|MakeRotator (.roll _returnvalue) (.pitch _returnvalue) 0.0))
  (Modes|PreviewMode false)
  (Widget|RemovefromParent (Variables|Default|GetW_EditMode))
  (Variables|Default|SetW_EditMode 0))

(fn SetPreviewColor
  (params (ColorPreview :type Enum_PreviewColor%20Enum :default "NewEnumerator0"))
  (bind _returnvalue (Actor|GetComponentsByClass "/Script/Engine.StaticMeshComponent"))
  (bind _grounded (Variables|Stats|GetGrounded))
  (bind _returnvalue_2 (Math|Conversions|ToFloat(Integer) _grounded))
  (switch Utilities|FlowControl|Switch|SwitchonEnum_PreviewColor ColorPreview
    (:NewEnumerator0
      (for _array_element _returnvalue
        (Rendering|Material|SetVectorParameterValueonMaterials _array_element "BuildingPreviewColor" "1.000000, 0, 0")))
    (:NewEnumerator1
      (for _array_element_2 _returnvalue
        (Rendering|Material|SetVectorParameterValueonMaterials _array_element_2 "BuildingPreviewColor" "0.100000,0.100000,1.000000")))
    (:NewEnumerator2
      (for _array_element_3 _returnvalue
        (Rendering|Material|SetVectorParameterValueonMaterials _array_element_3 "BuildingPreviewColor" (Math|Vector|MakeVector (Math|Float|MapRangeClamped _returnvalue_2 0.0 6.0 0.0 0.85) (Math|Float|MapRangeClamped _returnvalue_2 0.0 6.0 1.0 0.25) 0.0))))))

(fn AddOffsettoActor
  (params (Offset :type Vector))
  (bind _scene (Variables|Default|GetScene))
  (return (+ (Transformation|GetActorLocation) (* (Math|Vector|GetForwardVector _scene) (.x Offset)) (* (Math|Vector|GetRightVector _scene) (.y Offset)) (* (Math|Vector|GetUpVector _scene) (.z Offset)))))

(fn CheckPlacing
  (return false 0 false))

(fn ZeroDependsDestroy
  (for _array_element (Variables|ConnectionBuildings|GetSupports)
    (Utilities|Array|RemoveItem (Variables|BuildingActor_C|GetDepends _array_element) self)
    (if (<= (Utilities|Array|Length (Variables|BuildingActor_C|GetDepends _array_element)) 0)
      (CallFunction|ZeroDependsDestroy _array_element)))
  (Actor|DestroyActor))

(fn GetACInteract
  (return (Variables|Default|GetAC_Interact)))

(fn GetBuildingActor
  (return self))

(fn GetInteractionLocation
  (return "0, 0, 0"))

(fn INT1Client
  (params (InteractedPawn :type Pawn%20Object%20Reference) (InteractedPC_Sky :type PC%20Sky%20Object%20Reference) (InteractedWith :type IC%20Class%20Reference))
  (return false))

(fn INT1ClientInterrupt
  (params (InteractedPawn :type Pawn%20Object%20Reference) (InteractedPC_Sky :type PC%20Sky%20Object%20Reference) (InteractedWith :type IC%20Class%20Reference))
  (return false))

(fn INT1Server
  (params (InteractedPawn :type Pawn%20Object%20Reference) (InteractedPC_Sky :type PC%20Sky%20Object%20Reference) (InteractedWith :type IC%20Class%20Reference))
  (Development|PrintString "REPAIR BUILDING")
  (return true))

(fn INT1ServerInterrupt
  (params (InteractedPawn :type Pawn%20Object%20Reference) (InteractedPC_Sky :type PC%20Sky%20Object%20Reference) (InteractedWith :type IC%20Class%20Reference))
  (return false))

(fn INT2Client
  (params (InteractedPawn :type Pawn%20Object%20Reference) (InteractedPC_Sky :type PC%20Sky%20Object%20Reference) (InteractedWith :type IC%20Class%20Reference))
  (Default|EnableProlongedEdit (Variables|Default|GetAC_Interact) InteractedPawn)
  (bind _returnvalue (UserInterface|CreateWidget "/Game/Widgets/W_EditMode.W_EditMode_C" 0 self (Variables|/Game/Blueprints/PC_Sky.PC_Sky_C|GetPF_Normal InteractedPC_Sky)))
  (bind _output_get (Variables|Default|SetW_EditMode _returnvalue))
  (UserInterface|Viewport|AddtoViewport _output_get 0)
  (Modes|PreviewMode true)
  (return true))

(fn INT2ClientInterrupt
  (params (InteractedPawn :type Pawn%20Object%20Reference) (InteractedPC_Sky :type PC%20Sky%20Object%20Reference) (InteractedWith :type IC%20Class%20Reference))
  (Edit|DiscardEdit)
  (return true))

(fn INT2Server
  (params (InteractedPawn :type Pawn%20Object%20Reference) (InteractedPC_Sky :type PC%20Sky%20Object%20Reference) (InteractedWith :type IC%20Class%20Reference))
  (return false))

(fn INT2ServerInterrupt
  (params (InteractedPawn :type Pawn%20Object%20Reference) (InteractedPC_Sky :type PC%20Sky%20Object%20Reference) (InteractedWith :type IC%20Class%20Reference))
  (return false))

(fn INT3Client
  (params (InteractedPawn :type Pawn%20Object%20Reference) (InteractedPC_Sky :type PC%20Sky%20Object%20Reference) (InteractedWith :type IC%20Class%20Reference))
  (return false))

(fn INT3ClientInterrupt
  (params (InteractedPawn :type Pawn%20Object%20Reference) (InteractedPC_Sky :type PC%20Sky%20Object%20Reference) (InteractedWith :type IC%20Class%20Reference))
  (return false))

(fn INT3Server
  (params (InteractedPawn :type Pawn%20Object%20Reference) (InteractedPC_Sky :type PC%20Sky%20Object%20Reference) (InteractedWith :type IC%20Class%20Reference))
  (bind _ac_inventory (Class|BPIGeneral|GetInventory(Message) InteractedPawn))
  (bind _returnvalue (Utilities|GetDataTableRow "/Game/Blueprints/Building/DT_Buildings.DT_Buildings" (.rowname (Variables|Default|GetBuildingRow)))
    (:then
      (for _array_element (.Required (Utilities|Struct|BreakS_Building _returnvalue))
        (bind _success (Default|AddtoInventory _ac_inventory _array_element))
        (if _success
          _)))
    (:RowNotFound
      (CallFunction|A1PrintError (Utilities|String|Append "BUILDING ROW IS CORRUPTED: " (Utilities|GetDisplayName self)))))
  (Utilities|FlowControl|Sequence
    (:then_0
      (for _array_element_2 (Variables|ConnectionBuildings|GetSupports)
        (Utilities|Array|RemoveItem (Variables|BuildingActor_C|GetDepends _array_element_2) self)
        (if (<= (Utilities|Array|Length (Variables|BuildingActor_C|GetDepends _array_element_2)) 0)
          (CallFunction|ZeroDependsDestroy _array_element_2))))
    (:then_1
      (Utilities|FlowControl|Sequence
        (:then_0
          (for _array_element_3 (Variables|ConnectionBuildings|GetDepends)
            (Utilities|Array|RemoveItem (Variables|BuildingActor_C|GetSupports _array_element_3) self)))
        (:then_1
          (Actor|DestroyActor)
          (return true))))))

(fn INT3ServerInterrupt
  (params (InteractedPawn :type Pawn%20Object%20Reference) (InteractedPC_Sky :type PC%20Sky%20Object%20Reference) (InteractedWith :type IC%20Class%20Reference))
  (return false))