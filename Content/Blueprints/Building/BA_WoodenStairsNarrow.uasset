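; Building actor for narrow wooden stairs that validates its own placement and sets a preview color to match.
; The construction script runs CheckPlacing, a Visibility box trace along the underside, pitched to the stair slope and offset from the actor.
; Placement passes when the trace hits nothing or an actor tagged Island, and fails on any other hit.
; Both client and server INT1 interaction functions simply return false.
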(fn ConstructionScript
  (CallFunction|CheckPlacing))

(fn CheckPlacing
  (bind _returnvalue (Transformation|GetActorRotation))
  (bind (_outhit _returnvalue_2) (Collision|BoxTraceByChannel (CallFunction|AddOffsettoActor "125.000000,0.000000,-15.000000") (CallFunction|AddOffsettoActor "-90.000000,0.000000,-120.000000") "5.000000,40.000000,10.000000" (Math|Rotator|MakeRotator (.roll _returnvalue) 26.5 (.yaw _returnvalue)) "TraceTypeQuery1" false 0 "None" true "(R=1.000000,G=0.000000,B=0.000000,A=1.000000)" "(R=0.000000,G=1.000000,B=0.000000,A=1.000000)" 2.0))
  (if _returnvalue_2
    (if (Actor|ActorHasTag (.HitActor (Collision|BreakHitResult _outhit)) "Island")
      _
      (else
        (CallFunction|SetPreviewColor "NewEnumerator0")
        (return false 0))))
  (CallFunction|SetPreviewColor "NewEnumerator2")
  (return true 0))

(fn INT1Client
  (params (InteractedPawn :type Pawn%20Object%20Reference) (InteractedPC_Sky :type PC%20Sky%20Object%20Reference) (InteractedWith :type IC%20Class%20Reference))
  (return false))

(fn INT1Server
  (params (InteractedPawn :type Pawn%20Object%20Reference) (InteractedPC_Sky :type PC%20Sky%20Object%20Reference) (InteractedWith :type IC%20Class%20Reference))
  (return false))