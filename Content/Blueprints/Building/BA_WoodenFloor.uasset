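; BA_WoodenFloor is a wooden floor building piece with its own placement validity check.
; CheckPlacing sweeps a thin, actor-rotated box on the Visibility channel across the floor's footprint, with endpoints offset from the actor.
; A hit blocks placement and a clear trace allows it, each setting a preview color; Grounded is always false.
; It exposes its interact component, while both server and client interaction handlers return false.
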(fn ConstructionScript)

(fn CheckPlacing
  (bind _returnvalue (Collision|BoxTraceByChannel (CallFunction|AddOffsettoActor "140.000000,0.000000,0.000000") (CallFunction|AddOffsettoActor "-140.000000,0.000000,0.000000") "1.000000,140.000000,10.000000" (Transformation|GetActorRotation) "TraceTypeQuery1" false 0 "None" true "(R=1.000000,G=0.000000,B=0.000000,A=1.000000)" "(R=0.000000,G=1.000000,B=0.000000,A=1.000000)" 2.0))
  (if _returnvalue
    (CallFunction|SetPreviewColor "NewEnumerator0")
    (return false 0 false)
    (else
      (CallFunction|SetPreviewColor "NewEnumerator2")
      (return true 0 false))))

(fn GetACInteract
  (return (Variables|Default|GetAC_Interact)))

(fn INT3Server
  (params (InteractedPawn :type Pawn%20Object%20Reference) (InteractedPC_Sky :type PC%20Sky%20Object%20Reference) (InteractedWith :type IC%20Class%20Reference))
  (return false))

(fn INT3Client
  (params (InteractedPawn :type Pawn%20Object%20Reference) (InteractedPC_Sky :type PC%20Sky%20Object%20Reference) (InteractedWith :type IC%20Class%20Reference))
  (return false))