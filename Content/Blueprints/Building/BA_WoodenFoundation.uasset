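; Wooden foundation building actor that validates its own placement and colors its preview to show whether it can be placed.
; CheckPlacing fails if a box trace at its location hits anything, then traces down from four corners.
; All four must land on Island-tagged or all on BA_Foundation-tagged actors; only the Island case returns an actor to attach to.
; It also exposes its interact component and itself through getters.
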(fn ConstructionScript
  (|CallParentFunction))

(fn CheckPlacing
  (bind _returnvalue (Transformation|GetActorLocation))
  (LocalVariables|SetARot (Transformation|GetActorRotation))
  (bind _returnvalue_2 (Collision|BoxTraceByChannel _returnvalue _returnvalue "149.000000,149.000000,10.000000" (LocalVariables|GetARot) "TraceTypeQuery1" false 0 "None" true "(R=1.000000,G=0.000000,B=0.000000,A=1.000000)" "(R=0.000000,G=1.000000,B=0.000000,A=1.000000)" 2.0))
  (if _returnvalue_2
    (CallFunction|SetPreviewColor "NewEnumerator0")
    (return false 0)
    (else
      (bind (_outhit _returnvalue_3) (Collision|BoxTraceByChannel (CallFunction|AddOffsettoActor "125.000000,125.000000,-15.000000") (CallFunction|AddOffsettoActor "125.000000,125.000000,-280.000000") "15.000000,15.000000,10.000000" (LocalVariables|GetARot) "TraceTypeQuery1" false 0 "None" true "(R=1.000000,G=0.000000,B=0.000000,A=1.000000)" "(R=0.000000,G=1.000000,B=0.000000,A=1.000000)" 2.0))
      (bind (_outhit_2 _returnvalue_4) (Collision|BoxTraceByChannel (CallFunction|AddOffsettoActor "-125.000000,-125.000000,-15.000000") (CallFunction|AddOffsettoActor "-125.000000,-125.000000,-280.000000") "15.000000,15.000000,10.000000" (LocalVariables|GetARot) "TraceTypeQuery1" false 0 "None" true "(R=1.000000,G=0.000000,B=0.000000,A=1.000000)" "(R=0.000000,G=1.000000,B=0.000000,A=1.000000)" 2.0))
      (bind (_outhit_3 _returnvalue_5) (Collision|BoxTraceByChannel (CallFunction|AddOffsettoActor "125.000000,-125.000000,-15.000000") (CallFunction|AddOffsettoActor "125.000000,-125.000000,-280.000000") "15.000000,15.000000,10.000000" (LocalVariables|GetARot) "TraceTypeQuery1" false 0 "None" true "(R=1.000000,G=0.000000,B=0.000000,A=1.000000)" "(R=0.000000,G=1.000000,B=0.000000,A=1.000000)" 2.0))
      (bind (_outhit_4 _returnvalue_6) (Collision|BoxTraceByChannel (CallFunction|AddOffsettoActor "-125.000000,125.000000,-15.000000") (CallFunction|AddOffsettoActor "-125.000000,125.000000,-280.000000") "15.000000,15.000000,10.000000" (LocalVariables|GetARot) "TraceTypeQuery1" false 0 "None" true "(R=1.000000,G=0.000000,B=0.000000,A=1.000000)" "(R=0.000000,G=1.000000,B=0.000000,A=1.000000)" 2.0))
      (if (Math|Boolean|ANDBoolean _returnvalue_6 _returnvalue_5 _returnvalue_4 _returnvalue_3)
        (if (or (Math|Boolean|ANDBoolean (Actor|ActorHasTag (.HitActor (Collision|BreakHitResult _outhit)) "Island") (Actor|ActorHasTag (.HitActor (Collision|BreakHitResult _outhit_2)) "Island") (Actor|ActorHasTag (.HitActor (Collision|BreakHitResult _outhit_3)) "Island") (Actor|ActorHasTag (.HitActor (Collision|BreakHitResult _outhit_4)) "Island")) (Math|Boolean|ANDBoolean (Actor|ActorHasTag (.HitActor (Collision|BreakHitResult _outhit)) "BA_Foundation") (Actor|ActorHasTag (.HitActor (Collision|BreakHitResult _outhit_2)) "BA_Foundation") (Actor|ActorHasTag (.HitActor (Collision|BreakHitResult _outhit_3)) "BA_Foundation") (Actor|ActorHasTag (.HitActor (Collision|BreakHitResult _outhit_4)) "BA_Foundation")))
          (CallFunction|SetPreviewColor "NewEnumerator2")
          (if (Math|Boolean|ANDBoolean (Actor|ActorHasTag (.HitActor (Collision|BreakHitResult _outhit)) "Island") (Actor|ActorHasTag (.HitActor (Collision|BreakHitResult _outhit_2)) "Island") (Actor|ActorHasTag (.HitActor (Collision|BreakHitResult _outhit_3)) "Island") (Actor|ActorHasTag (.HitActor (Collision|BreakHitResult _outhit_4)) "Island"))
            (return true (.HitActor (Collision|BreakHitResult _outhit_4)))
            (else
              (return true 0)))
          (else
            _)))
      (CallFunction|SetPreviewColor "NewEnumerator0")
      (return false 0))))

(fn GetACInteract
  (return (Variables|Default|GetAC_Interact)))

(fn GetBuildingActor
  (return self))