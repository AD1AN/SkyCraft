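; Pawn a player possesses to steer their flying island from an orbiting spring-arm camera scaled to island radius.
; Possession puts the player's Normal form in a spirit state and shows a control widget and Niagara direction indicator.
; Input sets direction, altitude and speed through server calls, with direction multicast and manual altitude also applied locally on clients.
; Exiting blends the view back and re-possesses the original pawn.
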(event Custom|HideCompleted
  (Widget|RemovefromParent (Variables|Default|GetW_PawnIslandControl)))

(event Custom|Multicast_OnPossess
  (params (PawnInControl :type Pawn%20Object%20Reference) (PlayerInControl :type BP%20PSS%20Object%20Reference))
  (Variables|Default|SetPawnInControl PawnInControl)
  (Variables|Default|SetPlayerInControl PlayerInControl)
  (switch Utilities|FlowControl|Switch|SwitchonEPlayerForm (Variables|/Script/SkyCraft.PSS|GetPlayerForm PlayerInControl)
    (:Normal
      (Variables|/Game/Blueprints/PF_Normal.PF_Normal_C|SetAnimSpirit (Variables|/Game/Blueprints/BP_PSS.BP_PSS_C|GetPF_Normal (Variables|Default|GetPlayerInControl)) true)
      (Variables|/Game/Blueprints/PF_Normal.PF_Normal_C|SetAnimLookAt (Variables|/Game/Blueprints/BP_PSS.BP_PSS_C|GetPF_Normal (Variables|Default|GetPlayerInControl)) false)
      (Variables|/Game/Blueprints/PF_Normal.PF_Normal_C|SetcanMove (Variables|/Game/Blueprints/BP_PSS.BP_PSS_C|GetPF_Normal (Variables|Default|GetPlayerInControl)) false)
      (Variables|/Game/Blueprints/PF_Normal.PF_Normal_C|SetcanQSPressing (Variables|/Game/Blueprints/BP_PSS.BP_PSS_C|GetPF_Normal (Variables|Default|GetPlayerInControl)) false)
      (Variables|/Game/Blueprints/PF_Normal.PF_Normal_C|SetcanInteract (Variables|/Game/Blueprints/BP_PSS.BP_PSS_C|GetPF_Normal (Variables|Default|GetPlayerInControl)) false)
      (Default|SetQSI (Variables|/Game/Blueprints/BP_PSS.BP_PSS_C|GetPF_Normal (Variables|Default|GetPlayerInControl)) -1))))

(event Custom|OnTargetDirection_Event
  (bind _bp_playerisland (Variables|Default|GetBP_PlayerIsland))
  (Niagara|SetNiagaraVariable(Vector3) (Variables|/Game/Blueprints/BP_PlayerIsland.BP_PlayerIsland_C|GetNS_Direction (Variables|Default|GetBP_PlayerIsland)) "IslandDirection" (Math|Vector|SelectVector "0, 0, 0" (* (Variables|/Script/SkyCraft.PlayerIsland|GetTargetDirection _bp_playerisland) (* (Variables|/Script/SkyCraft.Island|GetShapeRadius _bp_playerisland) (Math|Float|MapRangeClamped (Variables|/Script/SkyCraft.Island|GetIslandSize _bp_playerisland) 0.0 1.0 3.0 1.5))) (Variables|/Script/SkyCraft.PlayerIsland|GetbStopIsland _bp_playerisland))))

(event Custom|Multicast_OnUnpossess
  (Utilities|FlowControl|Sequence
    (:then_0
      (switch Utilities|FlowControl|Switch|SwitchonEPlayerForm (Variables|/Script/SkyCraft.PSS|GetPlayerForm (Variables|Default|GetPlayerInControl))
        (:Normal
          (Variables|/Game/Blueprints/PF_Normal.PF_Normal_C|SetAnimSpirit (Variables|/Game/Blueprints/BP_PSS.BP_PSS_C|GetPF_Normal (Variables|Default|GetPlayerInControl)) false))))
    (:then_1
      (Variables|Default|SetPlayerInControl 0) ; Empty
      (Variables|Default|SetPawnInControl 0) ; Empty
    )))

(event Custom|Server_Exit
  (Game|Player|SetViewTargetwithBlend (Variables|/Game/Blueprints/BP_PSS.BP_PSS_C|GetBP_PCS (Variables|Default|GetPlayerInControl)) (Variables|Default|GetPawnInControl) 1.0 "VTBlend_EaseInOut" 2.0 false)
  (Pawn|Possess (Variables|/Game/Blueprints/BP_PSS.BP_PSS_C|GetBP_PCS (Variables|Default|GetPlayerInControl)) (Variables|Default|GetPawnInControl))
  (CallFunction|MulticastonUnpossess))

(event Custom|Exit
  (Class|BPILookRotation|SetLookRotation(Message) (Variables|Default|GetPawnInControl) (Variables|Default|GetLookRotation))
  (CallFunction|ServerExit))

(event Custom|OnIslandSize_Event
  (CallFunction|SetCameraArmLength (+ (Variables|/Script/SkyCraft.Island|GetShapeRadius (Variables|Default|GetPlayerIsland)) 6e+03)))

(event Custom|Multicast_SetLookRotation
  (params (LookRotation :type Rotator))
  (bind (_roll _pitch _yaw) (Math|Rotator|BreakRotator LookRotation))
  (bind _output_get (Variables|Default|SetLookRotation (Math|Rotator|MakeRotator 0.0 (Math|Float|ClampAngle _pitch -9e+01 2.0) _yaw)))
  (Class|SkySpringArmComponent|SetPreviousDesiredRotation (Variables|Default|GetSkySpringArm) _output_get))

(event EventBeginPlay
  (bind _asbp_gss (Utilities|Casting|CastToBP_GSS (Game|GetGameState)))
  (Variables|Default|SetBP_GSS _asbp_gss)
  (Utilities|IsValid (Variables|Default|GetPlayerIsland)
    (:Is%20Valid
      (bind _asbp_player_island (Utilities|Casting|CastToBP_PlayerIsland (Variables|Default|GetPlayerIsland)))
      (bind _output_get (Variables|Default|SetBP_PlayerIsland _asbp_player_island))
      (EventDispatchers|AssignOnIslandSize _output_get (delegate Custom|OnIslandSize_Event))
      (CallFunction|OnIslandSizeEvent))
    (:Is%20Not%20Valid
      (Variables|Default|SetFailedIslandArchon true))))

(event EventTick
  (params (DeltaSeconds :type Float%20%28single-precision%29))
  (Transformation|SetWorldRotation (Variables|Default|GetSkySpringArm) (Variables|Default|GetLookRotation) false false))

(event EventPossessed
  (params (NewController :type Controller%20Object%20Reference))
  (Game|Player|SetViewTargetwithBlend (Variables|/Game/Blueprints/BP_PSS.BP_PSS_C|GetBP_PCS (Variables|Default|GetPlayerInControl)) self 0.0 "VTBlend_Linear" 0.0 false))

(event EventOnRepPlayerIsland
  (if (Variables|Default|GetFailedIslandArchon)
    (bind _asbp_player_island (Utilities|Casting|CastToBP_PlayerIsland (Variables|Default|GetPlayerIsland)))
    (bind _output_get (Variables|Default|SetBP_PlayerIsland _asbp_player_island))
    (EventDispatchers|AssignOnIslandSize _output_get (delegate Custom|OnIslandSize_Event))
    (CallFunction|OnIslandSizeEvent)))

(event EventUnpossessed
  (params (OldController :type Controller%20Object%20Reference))
  (Actor|Tick|SetActorTickEnabled false))

(event EventClientUnpossessed
  (bind _w_pawnislandcontrol (Variables|Default|GetW_PawnIslandControl))
  (bind _anim_hide (Variables|/Game/Widgets/W_PawnIslandControl.W_PawnIslandControl_C|Getanim_hide _w_pawnislandcontrol))
  (Class|UserWidget|BindtoAnimationFinished _w_pawnislandcontrol _anim_hide (delegate Custom|HideCompleted))
  (UserInterface|Animation|PlayAnimation _w_pawnislandcontrol _anim_hide 0.0 1 "Forward" 1.0 false)
  (Components|Activation|SetActive (Variables|/Game/Blueprints/BP_PlayerIsland.BP_PlayerIsland_C|GetNS_Direction (Variables|Default|GetBP_PlayerIsland)) false false)
  (EventDispatchers|UnbindEventfromOnTargetDirection (Variables|Default|GetBP_PlayerIsland) (EventDispatchers|CreateEvent :!event Custom|OnTargetDirection_Event))
  (EventDispatchers|UnbindEventfromOnStopIsland (Variables|Default|GetBP_PlayerIsland) (EventDispatchers|CreateEvent :!event Custom|OnTargetDirection_Event)))

(event EventClientPossessed
  (bind _bp_playerisland (Variables|Default|GetBP_PlayerIsland))
  (Actor|Tick|SetActorTickEnabled true)
  (bind _returnvalue (UserInterface|CreateWidget "/Game/Widgets/W_PawnIslandControl.W_PawnIslandControl_C" 0 (Variables|Default|GetBP_PlayerIsland) (Variables|Default|GetPlayerInControl)))
  (bind _output_get (Variables|Default|SetW_PawnIslandControl _returnvalue))
  (UserInterface|Animation|PlayAnimation _output_get (Variables|/Game/Widgets/W_PawnIslandControl.W_PawnIslandControl_C|Getanim_show _output_get) 0.0 1 "Forward" 1.0 false)
  (UserInterface|Viewport|AddtoViewport (Variables|Default|GetW_PawnIslandControl) 0)
  (Components|Activation|SetActive (Variables|/Game/Blueprints/BP_PlayerIsland.BP_PlayerIsland_C|GetNS_Direction (Variables|Default|GetBP_PlayerIsland)) true false)
  (EventDispatchers|AssignOnTargetDirection (Variables|Default|GetBP_PlayerIsland) (delegate Custom|OnTargetDirection_Event))
  (EventDispatchers|BindEventtoOnStopIsland (Variables|Default|GetBP_PlayerIsland) (delegate Custom|OnTargetDirection_Event))
  (Niagara|SetNiagaraVariable(Vector3) (Variables|/Game/Blueprints/BP_PlayerIsland.BP_PlayerIsland_C|GetNS_Direction (Variables|Default|GetBP_PlayerIsland)) "IslandDirection" (Math|Vector|SelectVector "0, 0, 0" (* (Variables|/Script/SkyCraft.PlayerIsland|GetTargetDirection _bp_playerisland) (* (Variables|/Script/SkyCraft.Island|GetShapeRadius _bp_playerisland) (Math|Float|MapRangeClamped (Variables|/Script/SkyCraft.Island|GetIslandSize _bp_playerisland) 0.0 1.0 3.0 1.5))) (Variables|/Script/SkyCraft.PlayerIsland|GetbStopIsland _bp_playerisland))))

(event Custom|Server_SetTargetDirection
  (params (Target%20Direction :type Vector%20Net%20Quantize%20Normal%20Structure))
  (CallFunction|MulticastSetTargetDirection Target%20Direction)
  (Default|ServerUnstopIsland (Variables|Default|GetBP_PlayerIsland))
  (CallFunction|ClientSetTargetDirectionFX (Variables|/Script/SkyCraft.PlayerIsland|GetTargetDirection (Variables|Default|GetBP_PlayerIsland))))

(event Custom|Multicast_SetTargetDirection
  (params (Target%20Direction :type Vector%20Net%20Quantize%20Normal%20Structure))
  (Class|PlayerIsland|SetTargetDirection (Variables|Default|GetBP_PlayerIsland) Target%20Direction)
  (if (Variables|/Script/SkyCraft.PlayerIsland|GetbStopIsland (Variables|Default|GetBP_PlayerIsland))
    (Variables|/Script/SkyCraft.PlayerIsland|SetCurrentDirection (Variables|Default|GetBP_PlayerIsland) "") ; empty
  ))

(event Custom|Server_ManualAltitude
  (params (Up :type Boolean))
  (CallFunction|ManualAltitude Up))

(event Custom|Client_SetTargetDirectionFX
  (params (TargetDirection :type Vector%20Net%20Quantize%20Normal%20Structure))
  (Niagara|SpawnSystemAttached "/Game/Niagara/NS_IA_DirectionFire.NS_IA_DirectionFire" (Variables|/Script/Engine.Actor|GetRootComponent (Variables|Default|GetBP_PlayerIsland)) "None" (* TargetDirection (Variables|/Script/SkyCraft.Island|GetShapeRadius (Variables|Default|GetBP_PlayerIsland))) (Math|Rotator|MakeRotator 0.0 0.0 (.yaw (Math|Conversions|RotationFromXVector TargetDirection))) "KeepRelativeOffset" true)
  (Audio|PlaySound2D "/Game/Audio/SFX/IA_Direction.IA_Direction" 1.0 1.0 0.0 0 0)
  (Default|CallSetDirection))

(event Custom|Server_SetTargetAltitude
  (params (TargetAltitude :type Float%20%28double-precision%29))
  (bind _bp_playerisland (Variables|Default|GetBP_PlayerIsland))
  (bind _bp_gss (Variables|Default|GetBP_GSS))
  (bind _traversalaltitude (Variables|/Script/SkyCraft.GSS|GetTraversalAltitude _bp_gss))
  (bind _returnvalue (Class|PlayerIsland|SetTargetAltitude _bp_playerisland (Math|Float|Clamp(Float) TargetAltitude (.min _traversalaltitude) (.max _traversalaltitude))))
  (Class|PlayerIsland|SetAltitudeDirection (Variables|Default|GetBP_PlayerIsland) (select (> _returnvalue (.z (Transformation|GetActorLocation _bp_playerisland))) 1e+01 -1e+01)))

(event Input|EnhancedActionEvents|EnhancedInputActionInteract1
  (params (ActionValue :type Boolean) (ElapsedSeconds :type Float%20%28double-precision%29) (TriggeredSeconds :type Float%20%28double-precision%29) (InputAction :type Input%20Action%20Object%20Reference :default "/Game/Misc/EnhancedInput/Interact1.Interact1"))
  (:Started
    (Default|CreateMenu (Variables|Default|GetBP_PlayerIsland) self (Variables|Default|GetPlayerInControl))))

(event Input|EnhancedActionEvents|EnhancedInputActionWheelBoth
  (params (ActionValue :type Float%20%28double-precision%29) (ElapsedSeconds :type Float%20%28double-precision%29) (TriggeredSeconds :type Float%20%28double-precision%29) (InputAction :type Input%20Action%20Object%20Reference :default "/Game/Misc/EnhancedInput/WheelBoth.WheelBoth"))
  (bind _bp_playerisland (Variables|Default|GetBP_PlayerIsland))
  (if (Input|EnhancedActionValues|GetShift)
    (CallFunction|SetCameraArmLength (+ (Variables|/Script/Engine.SpringArmComponent|GetTargetArmLength (Variables|Default|GetSkySpringArm)) (* ActionValue -3e+02)))
    (elif (Input|EnhancedActionValues|GetAlt)
      (CallFunction|ServerSetTargetAltitude (+ (Variables|/Script/SkyCraft.PlayerIsland|GetTargetAltitude (Variables|Default|GetBP_PlayerIsland)) (* ActionValue 5e+02)))
      (elif (Variables|/Game/Blueprints/BP_PlayerIsland.BP_PlayerIsland_C|GetEssenceDeficit _bp_playerisland)
        (Default|ShowWarning (Variables|Default|GetPlayerInControl) "EssenceDeficit")
        (else
          (Default|ServerIASpeedChange (Variables|Default|GetPlayerInControl) (>= ActionValue 0.0) _bp_playerisland))))))

(event Input|EnhancedActionEvents|EnhancedInputActionDropItem
  (params (ActionValue :type Boolean) (ElapsedSeconds :type Float%20%28double-precision%29) (TriggeredSeconds :type Float%20%28double-precision%29) (InputAction :type Input%20Action%20Object%20Reference :default "/Game/Misc/EnhancedInput/DropItem.DropItem"))
  (:Started
    (CallFunction|Exit)))

(event Input|EnhancedActionEvents|EnhancedInputActionPhantomForm
  (params (ActionValue :type Boolean) (ElapsedSeconds :type Float%20%28double-precision%29) (TriggeredSeconds :type Float%20%28double-precision%29) (InputAction :type Input%20Action%20Object%20Reference :default "/Game/Misc/EnhancedInput/PhantomForm.PhantomForm"))
  (:Started
    (Default|ServerToggleStopIA (Variables|Default|GetPlayerInControl))))

(event Input|EnhancedActionEvents|EnhancedInputActionCameraRotate
  (params (ActionValue :type Vector%202D%20Structure) (ElapsedSeconds :type Float%20%28double-precision%29) (TriggeredSeconds :type Float%20%28double-precision%29) (InputAction :type Input%20Action%20Object%20Reference :default "/Game/Misc/EnhancedInput/CameraRotate.CameraRotate"))
  (bind (_x _y) (Math|Vector2D|BreakVector2D ActionValue))
  (bind _bp_gss (Variables|Default|GetBP_GSS))
  (bind _bp_gis (Variables|/Game/Blueprints/BP_GSS.BP_GSS_C|GetBP_GIS _bp_gss))
  (bind _old_localsettings (Variables|/Game/Blueprints/BP_GIS.BP_GIS_C|GetOLD_LocalSettings _bp_gis))
  (bind _camerasensetivity (Variables|/Game/Blueprints/OLD_LocalSettings.OLD_LocalSettings_C|GetCameraSensetivity _old_localsettings))
  (Variables|Default|SetLookRotation (Math|Rotator|MakeRotator (.roll (Variables|Default|GetLookRotation)) (Math|Float|ClampAngle (+ (* _y _camerasensetivity (select (Variables|/Game/Blueprints/OLD_LocalSettings.OLD_LocalSettings_C|GetInvertVerticalMouse _old_localsettings) -1.0 1.0)) (.pitch (Variables|Default|GetLookRotation))) -9e+01 2.0) (+ (* _x _camerasensetivity) (.yaw (Variables|Default|GetLookRotation))))))

(event Input|EnhancedActionEvents|EnhancedInputActionLMB
  (params (ActionValue :type Boolean) (ElapsedSeconds :type Float%20%28double-precision%29) (TriggeredSeconds :type Float%20%28double-precision%29) (InputAction :type Input%20Action%20Object%20Reference :default "/Game/Misc/EnhancedInput/LMB.LMB"))
  (:Started
    (CallFunction|ServerSetTargetDirection (Class|AdianFL|ToQuantizeNormal(Vector) (Math|Vector|GetForwardVector (Math|Rotator|MakeRotator 0.0 0.0 (.yaw (Variables|Default|GetLookRotation))))))))

(event Input|EnhancedActionEvents|EnhancedInputActionMoveVertical
  (params (ActionValue :type Float%20%28double-precision%29) (ElapsedSeconds :type Float%20%28double-precision%29) (TriggeredSeconds :type Float%20%28double-precision%29) (InputAction :type Input%20Action%20Object%20Reference :default "/Game/Misc/EnhancedInput/MoveVertical.MoveVertical"))
  (bind _returnvalue (> ActionValue 0.0))
  (CallFunction|ServerManualAltitude _returnvalue)
  (if (and (not (Networking|IsServer)) (Pawn|IsLocallyControlled))
    (CallFunction|ManualAltitude _returnvalue)))

(event Input|EnhancedActionEvents|EnhancedInputActionMove2D
  (params (ActionValue :type Vector%202D%20Structure) (ElapsedSeconds :type Float%20%28double-precision%29) (TriggeredSeconds :type Float%20%28double-precision%29) (InputAction :type Input%20Action%20Object%20Reference :default "/Game/Misc/EnhancedInput/Move2D.Move2D"))
  (bind (_x _y) (Math|Vector2D|BreakVector2D ActionValue))
  (bind _lookrotation (Variables|Default|GetLookRotation))
  (:Triggered
    (Utilities|FlowControl|DoOnce false :!label _label
      (:Completed
        (CallFunction|ServerSetTargetDirection (Class|AdianFL|ToQuantizeNormal(Vector) (+ (* (Math|Vector|GetRightVector (Math|Rotator|MakeRotator 0.0 0.0 (.yaw _lookrotation))) _x) (* (Math|Vector|GetForwardVector (Math|Rotator|MakeRotator 0.0 0.0 (.yaw _lookrotation))) _y)))))))
  (:Completed
    (goto _label Reset)))

(event Input|EnhancedActionEvents|EnhancedInputActionInventory
  (params (ActionValue :type Boolean) (ElapsedSeconds :type Float%20%28double-precision%29) (TriggeredSeconds :type Float%20%28double-precision%29) (InputAction :type Input%20Action%20Object%20Reference :default "/Game/Misc/EnhancedInput/Inventory.Inventory"))
  (bind _playerincontrol (Variables|Default|GetPlayerInControl))
  (bind _returnvalue (UserInterface|CreateWidget "/Game/Widgets/CWS/CWS_UseAstralons.CWS_UseAstralons_C"))
  (UserInterface|Viewport|AddtoViewport _returnvalue 10)
  (Default|AddCWS _playerincontrol _returnvalue true true true "NewEnumerator2")
  (Default|SetMousetoCenter _playerincontrol))

(fn ConstructionScript)

(fn OnRepPlayerinControl
  (Default|CallOnPlayerinControl))

(fn SetCameraArmLength
  (params (NewLength :type Float%20%28double-precision%29))
  (bind _bp_playerisland (Variables|Default|GetBP_PlayerIsland))
  (bind _shaperadius (Variables|/Script/SkyCraft.Island|GetShapeRadius _bp_playerisland))
  (Variables|/Script/Engine.SpringArmComponent|SetTargetArmLength (Variables|Default|GetSkySpringArm) (Math|Float|Clamp(Float) NewLength (+ _shaperadius 1e+03) (+ _shaperadius 5e+03))))

(fn ManualAltitude
  (params (Up :type Boolean))
  (bind _bp_playerisland (Variables|Default|GetBP_PlayerIsland))
  (bind _bp_gss (Variables|Default|GetBP_GSS))
  (bind _traversalaltitude (Variables|/Script/SkyCraft.GSS|GetTraversalAltitude _bp_gss))
  (bind _altitudedirection (Variables|/Script/SkyCraft.PlayerIsland|GetAltitudeDirection _bp_playerisland))
  (Class|PlayerIsland|SetAltitudeDirection _bp_playerisland (select Up 3e+01 -3e+01))
  (Class|PlayerIsland|SetTargetAltitude (Variables|Default|GetBP_PlayerIsland) (Math|Float|Clamp(Float) (+ (+ _altitudedirection (* _altitudedirection (Variables|/Script/SkyCraft.PlayerIsland|GetCurrentSpeed _bp_playerisland) 0.005)) (.z (Transformation|GetActorLocation (Variables|Default|GetBP_PlayerIsland)))) (.min _traversalaltitude) (.max _traversalaltitude))))