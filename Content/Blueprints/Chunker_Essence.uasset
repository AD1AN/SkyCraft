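; Actor component that streams Chunk_Essence actors in a circular range around its owner, with tick enabled by the authority.
; When the owner crosses into a new chunk cell, it releases out-of-range chunks and claims or spawns those in range.
; Chunks are shared through a game mode registry and reference-counted by HMPR, which this component only decrements on release.
; Helpers release all claims or copy them from another generator.
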(event EventBeginPlay
  (Networking|SwitchHasAuthority
    (:Authority
      (bind _asbp_gis (Utilities|Casting|CastToBP_GIS (Game|GetGameInstance)))
      (Variables|Default|SetBP_GIS _asbp_gis)
      (bind _asbp_gms (Utilities|Casting|CastToBP_GMS (Game|GetGameMode)))
      (Variables|Default|SetBP_GMS _asbp_gms)
      (if (Class|LowEntryExtendedStandardLibrary|ShippingBuild)
        _
        (elif (Variables|/Game/Blueprints/BP_GIS.BP_GIS_C|GetisTestChunkEssenceRenderRange (Variables|Default|GetBP_GIS))
          (Variables|Default|SetRenderRange (Variables|/Game/Blueprints/BP_GIS.BP_GIS_C|GetTestChunkEssenceRenderRange (Variables|Default|GetBP_GIS)))))
      (Components|Tick|SetComponentTickEnabled true))))

(event EventTick
  (params (DeltaSeconds :type Float%20%28single-precision%29))
  (bind (_x _y) (CallFunction|GetActorChunkCors))
  (bind (_x_2 _y_2) (CallFunction|GetActorChunkCors))
  (if (not (and (== _x_2 (.x (Variables|Default|GetLastActorChunkCors))) (== _y_2 (.y (Variables|Default|GetLastActorChunkCors)))))
    (Variables|Default|SetLastActorChunkCors (Utilities|Struct|MakeCoords _x _y))
    (CallFunction|DestroyChunks)
    (CallFunction|SpawnChunks)))

(fn GetActorChunkCors
  (bind _returnvalue (Components|GetOwner))
  (bind _chunksizexy (Variables|Default|GetChunkSizeXY))
  (bind _returnvalue_2 (Transformation|GetActorLocation _returnvalue))
  (bind _returnvalue_3 (/ _returnvalue_2 _chunksizexy))
  (bind (_x _y) (Math|Vector|BreakVector _returnvalue_3))
  (return (Math|Float|Round _x) (Math|Float|Round _y)))

(fn DestroyChunks
  (bind (_x _y) (CallFunction|GetActorChunkCors))
  (bind _chunksizexy (Variables|Default|GetChunkSizeXY))
  (bind _chunksizexy_2 (Variables|Default|GetChunkSizeXY))
  (for (_array_element _array_index) (Variables|Default|GetHMPR_SpawnedChunkEssenceCors)
    (LocalVariables|SetTempIndex _array_index)
    (if (>= (Math|Vector|Distance(Vector) (Math|Vector|MakeVector (* (.X (Utilities|Struct|BreakCoords _array_element)) _chunksizexy) (* (.Y (Utilities|Struct|BreakCoords _array_element)) _chunksizexy) 0.0) (Math|Vector|MakeVector (* _x _chunksizexy_2) (* _y _chunksizexy_2) 0.0)) (* (Variables|Default|GetRenderRange) (Variables|Default|GetChunkSizeXY)))
      (Utilities|Array|Add (LocalVariables|GetIndexForRemoval) (LocalVariables|GetTempIndex))))
  (for (_array_element_2 _array_index_2) (LocalVariables|GetIndexForRemoval)
    (Variables|/Game/Blueprints/Chunk_Essence.Chunk_Essence_C|SetHMPR (Utilities|Array|Get(acopy) (Variables|Default|GetHMPR_SpawnedChunkEssence) (- _array_element_2 _array_index_2)) (- (Variables|/Game/Blueprints/Chunk_Essence.Chunk_Essence_C|GetHMPR (Utilities|Array|Get(acopy) (Variables|Default|GetHMPR_SpawnedChunkEssence) (- _array_element_2 _array_index_2))) 1))
    (Utilities|Array|RemoveIndex (Variables|Default|GetHMPR_SpawnedChunkEssenceCors) (- _array_element_2 _array_index_2))
    (Utilities|Array|RemoveIndex (Variables|Default|GetHMPR_SpawnedChunkEssence) (- _array_element_2 _array_index_2))))

(fn SpawnChunks
  (bind (_x _y) (CallFunction|GetActorChunkCors))
  (bind _renderrange (Variables|Default|GetRenderRange))
  (bind _renderrange_2 (Variables|Default|GetRenderRange))
  (bind _chunksizexy (Variables|Default|GetChunkSizeXY))
  (bind _bp_gms (Variables|Default|GetBP_GMS))
  (bind _bp_gms_2 (Variables|Default|GetBP_GMS))
  (bind _chunksizexy_2 (Variables|Default|GetChunkSizeXY))
  (for _index (range (* _renderrange_2 -1) _renderrange_2)
    (LocalVariables|SetTempX _index)
    (for _index_2 (range (* _renderrange -1) _renderrange)
      (LocalVariables|SetTempY _index_2)
      (LocalVariables|SetChunkCoords (Utilities|Struct|MakeCoords (+ _x (LocalVariables|GetTempX)) (+ _y (LocalVariables|GetTempY))))
      (if (and (not (Utilities|Array|ContainsItem (Variables|Default|GetHMPR_SpawnedChunkEssenceCors) (LocalVariables|GetChunkCoords))) (< (Math|Vector|VectorLength (Math|Vector|MakeVector (* (LocalVariables|GetTempX) _chunksizexy) (* (LocalVariables|GetTempY) _chunksizexy) 0.0)) (* (Variables|Default|GetRenderRange) (Variables|Default|GetChunkSizeXY))))
        (if (Utilities|Array|ContainsItem (Variables|/Game/Blueprints/BP_GMS.BP_GMS_C|GetSpawnedChunkEssenceCoords (Variables|Default|GetBP_GMS)) (LocalVariables|GetChunkCoords))
          (Utilities|Array|Add (Variables|Default|GetHMPR_SpawnedChunkEssenceCors) (LocalVariables|GetChunkCoords))
          (Utilities|Array|Add (Variables|Default|GetHMPR_SpawnedChunkEssence) (Utilities|Array|Get(acopy) (Variables|/Game/Blueprints/BP_GMS.BP_GMS_C|GetSpawnedChunkEssence _bp_gms_2) (Utilities|Array|FindItem (Variables|/Game/Blueprints/BP_GMS.BP_GMS_C|GetSpawnedChunkEssenceCoords _bp_gms_2) (LocalVariables|GetChunkCoords))))
          (Variables|/Game/Blueprints/Chunk_Essence.Chunk_Essence_C|SetHMPR (Utilities|Array|Get(acopy) (Variables|/Game/Blueprints/BP_GMS.BP_GMS_C|GetSpawnedChunkEssence _bp_gms_2) (Utilities|Array|FindItem (Variables|/Game/Blueprints/BP_GMS.BP_GMS_C|GetSpawnedChunkEssenceCoords _bp_gms_2) (LocalVariables|GetChunkCoords))) (+ (Variables|/Game/Blueprints/Chunk_Essence.Chunk_Essence_C|GetHMPR (Utilities|Array|Get(acopy) (Variables|/Game/Blueprints/BP_GMS.BP_GMS_C|GetSpawnedChunkEssence _bp_gms_2) (Utilities|Array|FindItem (Variables|/Game/Blueprints/BP_GMS.BP_GMS_C|GetSpawnedChunkEssenceCoords _bp_gms_2) (LocalVariables|GetChunkCoords)))) 1))
          (else
            ;[1 1 1] SpawnChunk
            (bind _returnvalue (Game|SpawnActorfromClass "/Game/Blueprints/Chunk_Essence.Chunk_Essence_C" (Math|Transform|MakeTransform (Math|Vector|MakeVector (* (.x (LocalVariables|GetChunkCoords)) _chunksizexy_2) (* (.y (LocalVariables|GetChunkCoords)) _chunksizexy_2) 9e+04) "0, 0, 0" "1.000000,1.000000,1.000000") "AlwaysSpawn" "OverrideRootScale" 0 (Variables|Default|GetBP_GMS) 1 0))
            (Utilities|Array|Add (Variables|/Game/Blueprints/BP_GMS.BP_GMS_C|GetSpawnedChunkEssence _bp_gms) _returnvalue)
            (Utilities|Array|Add (Variables|/Game/Blueprints/BP_GMS.BP_GMS_C|GetSpawnedChunkEssenceCoords _bp_gms) (LocalVariables|GetChunkCoords))
            (Utilities|Array|Add (Variables|Default|GetHMPR_SpawnedChunkEssence) _returnvalue)
            (Utilities|Array|Add (Variables|Default|GetHMPR_SpawnedChunkEssenceCors) (LocalVariables|GetChunkCoords))))))))

(fn MinusSpawnedChunks
  (for _array_element (Variables|Default|GetHMPR_SpawnedChunkEssence)
    (Variables|/Game/Blueprints/Chunk_Essence.Chunk_Essence_C|SetHMPR _array_element (- (Variables|/Game/Blueprints/Chunk_Essence.Chunk_Essence_C|GetHMPR _array_element) 1)))
  (Utilities|Array|Clear (Variables|Default|GetHMPR_SpawnedChunkEssence))
  (Utilities|Array|Clear (Variables|Default|GetHMPR_SpawnedChunkEssenceCors)))

(fn TransferChunks
  (params (FromGenerator :type Chunker%20Essence%20Object%20Reference))
  (Variables|Default|SetHMPR_SpawnedChunkEssence (Variables|Chunker_Essence_C|GetHMPR_SpawnedChunkEssence FromGenerator))
  (Variables|Default|SetHMPR_SpawnedChunkEssenceCors (Variables|Chunker_Essence_C|GetHMPR_SpawnedChunkEssenceCors FromGenerator))
  (Variables|Default|SetLastActorChunkCors (Variables|Chunker_Essence_C|GetLastActorChunkCors FromGenerator))
  (return))