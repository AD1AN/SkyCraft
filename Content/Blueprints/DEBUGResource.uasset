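; Debug resource actor that gives one Stone to the interacting player's inventory through a server-side interact handler.
; A successful insert destroys the actor, while a failed insert calls Die on a HealthSystem.
; The client interact and both interrupt handlers are stubs that return false.
; On BeginPlay it draws a long-lived debug box above itself and scatters debug spheres at random points inside that volume.
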(event EventBeginPlay
  (bind _returnvalue (Transformation|GetActorLocation))
  (bind _returnvalue_2 (+ _returnvalue "0.000000,0.000000,300.000000"))
  (Rendering|Debug|DrawDebugBox _returnvalue_2 "10.000000,10.000000,200.000000" "(R=1.000000,G=0.000000,B=0.081863,A=1.000000)" "0, 0, 0" 555.0 0.0)
  (for _index (range 0 22)
    (Rendering|Debug|DrawDebugSphere (Math|Random|RandomPointinBoundingBox _returnvalue_2 "10.000000,10.000000,200.000000") 2.0 12 "(R=1.000000,G=1.000000,B=1.000000,A=1.000000)" 5555.0)))

(fn ConstructionScript)

(fn ClientInteractBP
  (params (InteractKey :type EInteractKey%20Enum :default "Interact1") (Pawn :type Pawn%20Object%20Reference) (BP_PAI :type BP%20PAI%20Object%20Reference))
  (return false))

(fn ClientInterruptBP
  (params (InterruptedBy :type EInterruptedBy%20Enum :default "Player") (InteractKey :type EInteractKey%20Enum :default "Interact1") (Pawn :type Pawn%20Object%20Reference) (BP_PAI :type BP%20PAI%20Object%20Reference))
  (return false))

(fn ServerInteractBP
  (params (InteractKey :type EInteractKey%20Enum :default "Interact1") (Pawn :type Pawn%20Object%20Reference) (BP_PAI :type BP%20PAI%20Object%20Reference))
  (bind _returnvalue (Class|Inventory|InsertSlot (Default|GetPlayerInventory BP_PAI) (Utilities|Struct|MakeSlot "/Game/DataAssets/Item/Stone.Stone" 1 0)))
  (if _returnvalue
    (Actor|DestroyActor)
    (return true)
    (else
      (Class|HealthSystem|Die (Variables|Default|GetHealthSystem) 0 "0, 0, 0"))))

(fn ServerInterruptBP
  (params (InterruptedBy :type EInterruptedBy%20Enum :default "Player") (InteractKey :type EInteractKey%20Enum :default "Interact1") (Pawn :type Pawn%20Object%20Reference) (BP_PAI :type BP%20PAI%20Object%20Reference))
  (return false))