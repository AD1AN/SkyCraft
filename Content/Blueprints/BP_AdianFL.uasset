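; BP_AdianFL is a function library of shared helpers for gameplay and local save data.
; LoadLocalSettings loads the LocalSettings save slot, creating it if missing and repairing an invalid character selection.
; When no character exists, CreateRandomCharacter adds one with random name, gender and appearance, then saves.
; Other helpers cover essence and vector math, seeded random integers, equipment slot mapping, array and property searches, and sky tags read from root-component asset user data.
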(fn SubtractEssence
  (params (1 :type Essence%20Structure) (2 :type Essence%20Structure))
  (bind (_r _g _b) (Utilities|Struct|BreakEssence 1))
  (bind (_r_2 _g_2 _b_2) (Utilities|Struct|BreakEssence 2))
  (return (Utilities|Struct|MakeEssence (- _r _r_2) (- _g _g_2) (- _b _b_2))))

(fn EssenceMax
  (params (Essence :type Essence%20Structure))
  (return (Math|Conversions|ToFloat(Integer) (Math|Integer|Max(Integer) (.r Essence) (.g Essence) (.b Essence)))))

(fn Int->Stream->Int
  (params (InitialSeed :type Integer))
  (return (Class|KismetMathLibrary|RandomIntegerfromStream (Math|Random|MakeRandomStream InitialSeed) 2147483647)))

(fn DistanceMeters
  (params (A :type Actor%20Object%20Reference) (B :type Actor%20Object%20Reference))
  (return (Math|Float|Truncate (/ (Math|Vector|Distance(Vector) (Transformation|GetActorLocation A) (Transformation|GetActorLocation B)) 1e+02))))

(fn EquipmentType
  (params (SlotIndex :type Integer))
  (return (Utilities|Select :Index SlotIndex :Option%200 "EQHead" :Option%201 "EQOutfit" :Option%202 "EQHands" :Option%203 "EQFeet")))

(fn FindProperty
  (params (FindProperty :type DA%20Item%20Property%20Object%20Reference) (SearchInProperties :type Array%20of%20Item%20Property%20Structures))
  (bind (_array_element _array_index) (Utilities|Array|ForEachLoopwithBreak SearchInProperties)
    (:LoopBody
      (if (== (Utilities|Struct|BreakItemProperty _array_element) FindProperty)
        (return true _array_element _array_index)))
    (:Completed
      (return false "" 0))))

(fn AdianPrintError
  (params (Message :type String))
  (Development|PrintString 0 Message true true "(R=1.000000,G=0.000000,B=0.016666,A=1.000000)" 15.0))

(fn CreateRandomCharacter
  (params (LocalSettings :type Local%20Settings%20Object%20Reference))
  (bind _returnvalue (Math|Random|RandomInteger 9))
  (bind _returnvalue_2 (Math|Random|RandomBool))
  (bind _returnvalue_3 (Class|KismetSystemLibrary|MakeLiteralBool _returnvalue_2))
  (bind _returnvalue_4 (Utilities|Array|Add (Variables|/Game/Blueprints/LocalSettings.LocalSettings_C|GetCharactersBio LocalSettings) (Utilities|Struct|MakeCharacterBio (select _returnvalue_3 (Utilities|Select :Index _returnvalue :Option%200 "Lukas" :Option%201 "Wigmar" :Option%202 "Tullus" :Option%203 "Ellis" :Option%204 "Opiter" :Option%205 "Tertius" :Option%206 "Manius" :Option%207 "Nofri" :Option%208 "Lambertus" :Option%209 "Binet") (Utilities|Select :Index _returnvalue :Option%200 "Mary" :Option%201 "Sittia" :Option%202 "Nora" :Option%203 "Lorraine" :Option%204 "Eva" :Option%205 "Eileen" :Option%206 "Amelina" :Option%207 "Silia" :Option%208 "Plinia" :Option%209 "Vanessa")) _returnvalue_3 0 (Class|KismetMathLibrary|HSVtoRGB (Math|Random|RandomFloatinRange 0.0 3.6e+02) (Math|Random|RandomFloatinRange 0.0 0.75) (Math|Random|RandomFloatinRange 0.0 1.0) 1.0) (Class|KismetMathLibrary|HSVtoRGB (Math|Random|RandomFloatinRange 0.0 3.6e+02) (Math|Random|RandomFloatinRange 0.0 1.0) (Math|Random|RandomFloatinRange 0.25 1.0) 1.0) (Math|Random|RandomFloatinRange 0.9 1.0) (Math|DateTime|Now))))
  (Default|SetSelectedCharacterBioIndex LocalSettings _returnvalue_4)
  (SaveGame|SaveGametoSlot LocalSettings "LocalSettings")
  (return))

(fn LoadLocalSettings
  (Utilities|FlowControl|Sequence
    (:then_0
      (bind _returnvalue (SaveGame|DoesSaveGameExist "LocalSettings"))
      (if _returnvalue
        (bind _returnvalue_2 (SaveGame|LoadGamefromSlot "LocalSettings"))
        (bind _aslocal_settings (Utilities|Casting|CastToLocalSettings _returnvalue_2))
        (if (not (Utilities|Array|IsValidIndex (Variables|/Game/Blueprints/LocalSettings.LocalSettings_C|GetCharactersBio _aslocal_settings) (Default|GetSelectedCharacterBioIndex _aslocal_settings)))
          (if (Utilities|Array|IsEmpty (Variables|/Game/Blueprints/LocalSettings.LocalSettings_C|GetCharactersBio _aslocal_settings))
            (CallFunction|CreateRandomCharacter _aslocal_settings)
            (else
              (Default|SetSelectedCharacterBioIndex _aslocal_settings (Utilities|Array|LastIndex (Variables|/Game/Blueprints/LocalSettings.LocalSettings_C|GetCharactersBio _aslocal_settings)))
              (SaveGame|SaveGametoSlot _aslocal_settings "LocalSettings"))))
        (else
          (bind _returnvalue_3 (SaveGame|CreateSaveGameObject "/Game/Blueprints/LocalSettings.LocalSettings_C"))
          (CallFunction|CreateRandomCharacter _returnvalue_3 (LocalVariables|Get__WorldContext)))))
    (:then_1
      (bind _returnvalue_4 (SaveGame|LoadGamefromSlot "LocalSettings"))
      (bind _aslocal_settings_2 (Utilities|Casting|CastToLocalSettings _returnvalue_4))
      (return _aslocal_settings_2))))

(fn SaveLocalSettings
  (params (LocalSettings :type Local%20Settings%20Object%20Reference%20%28by%20ref%29))
  (SaveGame|SaveGametoSlot LocalSettings "LocalSettings"))

(fn VectorSignInvert
  (params (InVector :type Vector) (InvertX :type Boolean) (InvertY :type Boolean) (InvertZ :type Boolean))
  (bind (_x _y _z) (Math|Vector|BreakVector InVector))
  (return (Math|Vector|MakeVector (Math|Float|SelectFloat (* _x -1.0) _x InvertX) (Math|Float|SelectFloat (* _y -1.0) _y InvertY) (Math|Float|SelectFloat (* _z -1.0) _z InvertZ))))

(fn CombineArrays
  (params (From :type Array%20of%20Object%20Object%20References) (To :type Array%20of%20Object%20Object%20References))
  (for _array_element From
    (Utilities|Array|Add To _array_element)))

(fn ContainsTags
  (params (InArray :type Array%20of%20Names) (FindArray :type Array%20of%20Names))
  (for _array_element InArray
    (if (Utilities|Array|ContainsItem FindArray _array_element)
      (return true)))
  (return false))

(fn ArrayContainsSkyTag
  (params (SearchFor :type Array%20of%20DA%20Sky%20Tag%20Object%20References) (SearchIn :type Array%20of%20DA%20Sky%20Tag%20Object%20References))
  (for _array_element SearchFor
    (if (Utilities|Array|ContainsItem SearchIn _array_element)
      (return true _array_element)))
  (return false 0))

(fn PropertyEqual
  (params (Property1 :type DA%20Item%20Property%20Object%20Reference) (Property2 :type DA%20Item%20Property%20Object%20Reference))
  (return (== Property1 Property2)))

(fn ContainsProperty
  (params (Properties :type Array%20of%20Item%20Property%20Structures) (Property :type DA%20Item%20Property%20Object%20Reference))
  (for (_array_element _array_index) Properties
    (if (== (.property _array_element) Property)
      (return true _array_index)))
  (return false -1))

(fn GetSkyTags
  (params (Actor :type Actor%20Object%20Reference))
  (bind _returnvalue (Class|AdianFL|GetAssetUserData (Variables|/Script/Engine.Actor|GetRootComponent Actor) "/Script/SkyCraft.AUD_SkyTags"))
  (Utilities|IsValid _returnvalue
    (:Is%20Valid
      (return (Variables|/Script/SkyCraft.AUD_SkyTags|GetDA_SkyTags _returnvalue)))))