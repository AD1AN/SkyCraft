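; CustomSettingsSave is a save object that stores the list of character bios and tracks which one is selected.
; Accessors read or replace the selected bio; changing the selection or removing a bio saves to the "CustomSettings" slot, with removal shifting the index as needed.
; Selection changes and renames trigger notification calls, but renaming does not itself write to disk.
; Save getters return itself for custom settings and nothing for the world save.
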(fn SetSelectedCharacterBio
  (params (InCharacterBio :type Character%20Bio%20Structure%20%28by%20ref%29))
  (Utilities|Array|SetArrayElem (Variables|Default|GetCharactersBio) (Variables|Default|GetSelectedCharacterBioIndex) InCharacterBio)
  (return InCharacterBio))

(fn GetSelectedCharacterBio
  (return (Utilities|Array|Get(acopy) (Variables|Default|GetCharactersBio) (Variables|Default|GetSelectedCharacterBioIndex))))

(fn SetSelectedCharacterBioIndex
  (params (SelectedCharacterBioIndex :type Integer))
  (Variables|Default|SetSelectedCharacterBioIndex SelectedCharacterBioIndex)
  (SaveGame|SaveGametoSlot self "CustomSettings")
  (Default|CallSelectedCharacterChanged))

(fn GetSelectedCharacterBioIndex
  (return (Variables|Default|GetSelectedCharacterBioIndex)))

(fn RemoveCharacterBio
  (params (CharBio_Index :type Integer))
  (if (< CharBio_Index (Variables|Default|GetSelectedCharacterBioIndex))
    (Math|Integer|DecrementInt (Variables|Default|GetSelectedCharacterBioIndex)
      (:%20%20
        _)))
  (Utilities|Array|RemoveIndex (Variables|Default|GetCharactersBio) CharBio_Index)
  (SaveGame|SaveGametoSlot self "CustomSettings"))

(fn ChangeNameforSelected
  (params (NewName :type Name))
  (bind _structout (Utilities|Struct|SetmembersinCharacterBio (CallFunction|GetSelectedCharacterBio) NewName))
  (CallFunction|SetSelectedCharacterBio _structout)
  (Default|CallNameChanged))

(fn GetCustomSettingsSave
  (return self))

(fn GetWorldSave
  (return 0))