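; BP_DamageNumbers is a floating damage number actor that shows a Damage value through a widget component.
; Its CustomBeginPlay event converts the spawn position into the attach parent's local space and writes the value as integer text into W_DamageNumbers.
; The FlyUp timeline then raises the relative location along Z, so the number stays relative to its parent, and destroys the actor when finished.
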(event EventCustomBeginPlay
  (Variables|Default|SetSpawnLocation (Math|Transform|InverseTransformLocation (Transformation|GetActorTransform (Actor|GetAttachParentActor)) (Transformation|GetActorLocation)))
  (bind _asw_damage_numbers (Utilities|Casting|CastToW_DamageNumbers (UserInterface|GetWidget (Variables|Default|GetWidget))))
  (Rendering|Components|TextRender|SetText (Variables|/Game/Widgets/W_DamageNumbers.W_DamageNumbers_C|GetTextNumbers _asw_damage_numbers) (Utilities|Text|ToText(Integer) (Variables|Default|GetDamage) false false))
  (bind _newtrack_0 (Timeline|FlyUp PlayFromStart)
    (:Update
      (Transformation|SetActorRelativeLocation (+ (Variables|Default|GetSpawnLocation) (Math|Vector|MakeVector 0.0 0.0 (* _newtrack_0 5e+01))) false true))
    (:Finished
      (Actor|DestroyActor))))

(fn ConstructionScript)