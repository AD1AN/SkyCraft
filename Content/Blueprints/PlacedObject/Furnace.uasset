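; Placeable furnace that burns fuel to turn input items into output items, with a UI on interact and pickup back into the player's inventory.
; Fuel or input inventory changes run TryCook, which matches items against the fuel and output DataTables and starts the burn.
; Tick advances or rewinds cook progress, produces output and refuels.
; It also handles build-preview materials, box-trace placement checks and save/load of transform and inventories.
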(event Custom|SAE_Inventory_Fuel
  (params (ChangedIndex :type Integer))
  (CallFunction|TryCook))

(event Custom|SAE_Inventory_Input
  (params (ChangedIndex :type Integer))
  (CallFunction|TryCook))

(event Custom|Uncook
  (Variables|Default|SetCurrentCookTime (Math|Float|Clamp(Float) (- (Variables|Default|GetCurrentCookTime) (Utilities|Time|GetWorldDeltaSeconds)) 0.0 (Variables|Default|GetEndCookTime))) ; Uncook
)

(event EventBeginPlay
  (EventDispatchers|AssignSAEInventory (Variables|Default|GetInventory_Fuel) (delegate Custom|SAE_Inventory_Fuel))
  (EventDispatchers|AssignSAEInventory (Variables|Default|GetInventory_Input) (delegate Custom|SAE_Inventory_Input)))

(event EventTick
  (params (DeltaSeconds :type Float%20%28single-precision%29))
  (bind _output (Variables|Default|GetOutput))
  (bind _fuel (Variables|Default|GetFuel))
  (bind _inventory_fuel (Variables|Default|GetInventory_Fuel))
  (bind _fuel_2 (Variables|Default|GetFuel))
  (bind _inventory_input (Variables|Default|GetInventory_Input))
  (bind _output_2 (Utilities|Struct|BreakS_FurnaceOutput _output))
  (bind _fuel_3 (Utilities|Struct|BreakS_FurnaceFuel _fuel_2))
  (bind _slots (Variables|/Game/Blueprints/Inventory.Inventory_C|GetSlots _inventory_fuel))
  (bind _slots_2 (Variables|/Game/Blueprints/Inventory.Inventory_C|GetSlots _inventory_input))
  (bind _quantity (Utilities|Struct|BreakInventorySlot _fuel_3))
  (bind _da_item (Utilities|Struct|BreakInventorySlot _output_2))
  (bind _output_3 (Utilities|Array|Get(acopy) _slots))
  (bind _output_4 (Utilities|Array|Get(acopy) _slots_2))
  (bind _quantity_2 (Utilities|Struct|BreakInventorySlot _output_3))
  (if (> (Variables|Default|GetCurrentFuelTime) 0.0) ; Have fuel?
    (Variables|Default|SetCurrentFuelTime (- (Variables|Default|GetCurrentFuelTime) (Utilities|Time|GetWorldDeltaSeconds))) ; Burn fuel
    (Utilities|FlowControl|Sequence
      (:then_0
        (Utilities|IsValid (Utilities|Struct|BreakInventorySlot (Utilities|Array|Get(acopy) (Variables|/Game/Blueprints/Inventory.Inventory_C|GetSlots (Variables|Default|GetInventory_Input))))
          (:Is%20Valid
            (Variables|Default|SetCurrentCookTime (+ (Variables|Default|GetCurrentCookTime) (Utilities|Time|GetWorldDeltaSeconds))) ; Cooking
          )
          (:Is%20Not%20Valid
            (Variables|Default|SetCurrentCookTime (Math|Float|Clamp(Float) (- (Variables|Default|GetCurrentCookTime) (Utilities|Time|GetWorldDeltaSeconds)) 0.0 (Variables|Default|GetEndCookTime))) ; Uncook
          )))
      (:then_1
        (if (>= (Variables|Default|GetCurrentCookTime) (Variables|Default|GetEndCookTime)) ; COOKED?
          (bind _structout (Utilities|Struct|SetmembersinInventorySlot _output_4 (- (Utilities|Struct|BreakInventorySlot _output_4) 1)))
          (Default|ServerSAEInventory (Variables|Default|GetInventory_Input) 0 _structout)
          (Utilities|IsValid _da_item
            (:Is%20Valid
              (Utilities|FlowControl|Sequence
                (:then_0
                  (if (Variables|/Script/SkyCraft.DA_Item|GetStacking _da_item)
                    _
                    (else
                      (Default|ServerSAEInventory (Variables|Default|GetInventory_Output))))
                  (Default|ServerAddtoInventory (Variables|Default|GetInventory_Output) (.Output (Utilities|Struct|BreakS_FurnaceOutput (Variables|Default|GetOutput)))))
                (:then_1
                  (Variables|Default|SetCurrentCookTime 0.0))))
            (:Is%20Not%20Valid
              (CallFunction|AdianPrintError "ERROR: IDK WTF I JUST COOKED")))))
      (:then_2
        (if (<= (Variables|Default|GetCurrentFuelTime) 0.0) ; Fuel burnt out
          (Variables|Default|SetCurrentFuelTime 0.0)
          (if (Utilities|IsValid (Utilities|Struct|BreakInventorySlot (Utilities|Array|Get(acopy) (Variables|/Game/Blueprints/Inventory.Inventory_C|GetSlots (Variables|Default|GetInventory_Input))))) ; Input empty?
            (if (>= _quantity_2 _quantity)
              (bind _structout_2 (Utilities|Struct|SetmembersinInventorySlot _output_3 (- _quantity_2 _quantity)))
              (Default|ServerSAEInventory (Variables|Default|GetInventory_Fuel) 0 _structout_2)
              (Variables|Default|SetCurrentFuelTime (.fueltime _fuel))
              (Variables|Default|SetMaxFuelTime (.fueltime _fuel))
              (Variables|Default|SetFuelEfficiency (.fuelefficiency _fuel)))))))
    (else
      (CallFunction|Uncook))))

(fn ConstructionScript)

(fn PreviewMode
  (params (PreviewMode :type Boolean))
  (bind _returnvalue (Actor|GetComponentsByClass "/Script/Engine.StaticMeshComponent"))
  (if PreviewMode
    (for _array_element _returnvalue
      (Rendering|Material|SetMaterial _array_element 0 "/Game/GlobalMaterials/M_BuildingPreview.M_BuildingPreview"))
    (else
      (for (_array_element_2 _array_index) _returnvalue
        (Rendering|Material|SetMaterial _array_element_2 0 (Utilities|Array|Get(acopy) (Variables|Default|GetMeshMaterials) _array_index))))))

(fn CollisionMode
  (params (CollisionMode :type ECollisionEnabled%20Enum :default "NoCollision"))
  (Utilities|FlowControl|Sequence
    (:then_0
      (for _array_element (Actor|GetComponentsByClass "/Script/Engine.StaticMeshComponent")
        (Collision|SetCollisionEnabled _array_element CollisionMode)))
    (:then_1
      (for _array_element_2 (Actor|GetComponentsByClass "/Script/Engine.BoxComponent")
        (Collision|SetCollisionEnabled _array_element_2 CollisionMode)))))

(fn SetPreviewColor
  (params (ColorPreview :type E_BuildingPartPreviewColor%20Enum :default "NewEnumerator0"))
  (bind _returnvalue (Actor|GetComponentsByClass "/Script/Engine.StaticMeshComponent"))
  (switch Utilities|FlowControl|Switch|SwitchonE_BuildingPartPreviewColor ColorPreview
    (:NewEnumerator0
      (for _array_element _returnvalue
        (Rendering|Material|SetVectorParameterValueonMaterials _array_element "BuildingPreviewColor" "1.000000, 0, 0")))
    (:NewEnumerator1
      (for _array_element_2 _returnvalue
        (Rendering|Material|SetVectorParameterValueonMaterials _array_element_2 "BuildingPreviewColor" "1.000000,0.300000, 0")))
    (:NewEnumerator2
      (for _array_element_3 _returnvalue
        (Rendering|Material|SetVectorParameterValueonMaterials _array_element_3 "BuildingPreviewColor" "0.000000,1.000000, 0")))))

(fn CheckPlacing
  (bind _returnvalue (Transformation|GetActorLocation))
  (bind _returnvalue_2 (Collision|BoxTraceByChannel (+ _returnvalue "0,0,20.000000") (+ _returnvalue "0.000000,0.000000,6.000000") "40.000000,40.000000,1.000000" (Transformation|GetActorRotation) "TraceTypeQuery1" false 0 "None" true "(R=1.000000,G=0.000000,B=0.000000,A=1.000000)" "(R=0.000000,G=1.000000,B=0.000000,A=1.000000)" 2.0))
  (if _returnvalue_2
    (CallFunction|SetPreviewColor "NewEnumerator0")
    (return false)
    (else
      (CallFunction|SetPreviewColor "NewEnumerator2")
      (return true))))

(fn TryCook
  (bind _inventory_fuel (Variables|Default|GetInventory_Fuel))
  (bind _slots (Variables|/Game/Blueprints/Inventory.Inventory_C|GetSlots _inventory_fuel))
  (bind _output (Utilities|Array|Get(acopy) _slots))
  (Utilities|FlowControl|Sequence
    (:then_0
      (Utilities|IsValid (.da_item (Utilities|Array|Get(acopy) (Variables|/Game/Blueprints/Inventory.Inventory_C|GetSlots (Variables|Default|GetInventory_Fuel))))
        (:Is%20Valid
          (bind _outrownames (DataTable|GetDataTableRowNames "/Game/Blueprints/ItemComponents/Furnace/DT_FurnaceFuel.DT_FurnaceFuel"))
          (bind _array_element (Utilities|Array|ForEachLoopwithBreak _outrownames :!label _label)
            (:LoopBody
              (bind _returnvalue (Utilities|GetDataTableRow "/Game/Blueprints/ItemComponents/Furnace/DT_FurnaceFuel.DT_FurnaceFuel" _array_element)
                (:then
                  (Variables|Default|SetFuel _returnvalue)
                  (if (== (Utilities|Struct|BreakInventorySlot (Utilities|Struct|BreakS_FurnaceFuel _returnvalue)) (.da_item (Utilities|Array|Get(acopy) (Variables|/Game/Blueprints/Inventory.Inventory_C|GetSlots (Variables|Default|GetInventory_Fuel)))))
                    (LocalVariables|SetFuelFound true)
                    (goto _label Break)))))))
        (:Is%20Not%20Valid
          (return))))
    (:then_1
      (if (LocalVariables|GetFuelFound)
        (Utilities|IsValid (.da_item (Utilities|Array|Get(acopy) (Variables|/Game/Blueprints/Inventory.Inventory_C|GetSlots (Variables|Default|GetInventory_Input))))
          (:Is%20Valid
            (bind _outrownames_2 (DataTable|GetDataTableRowNames "/Game/Blueprints/ItemComponents/Furnace/DT_FurnaceOutput.DT_FurnaceOutput"))
            (bind _array_element_2 (Utilities|Array|ForEachLoopwithBreak _outrownames_2 :!label _label_2)
              (:LoopBody
                (bind _returnvalue_2 (Utilities|GetDataTableRow "/Game/Blueprints/ItemComponents/Furnace/DT_FurnaceOutput.DT_FurnaceOutput" _array_element_2)
                  (:then
                    (Variables|Default|SetOutput _returnvalue_2)
                    (if (== (.DA_Item (Utilities|Struct|BreakInventorySlot (.Input (Utilities|Struct|BreakS_FurnaceOutput _returnvalue_2)))) (.da_item (Utilities|Array|Get(acopy) (Variables|/Game/Blueprints/Inventory.Inventory_C|GetSlots (Variables|Default|GetInventory_Input)))))
                      (LocalVariables|SetOutputFound true)
                      (goto _label_2 Break)))))))
          (:Is%20Not%20Valid
            (return)))
        (else
          (return))))
    (:then_2
      (if (and (LocalVariables|GetFuelFound) (LocalVariables|GetOutputFound))
        (Utilities|FlowControl|Sequence
          (:then_0
            (if (not (> (Variables|Default|GetCurrentFuelTime) 0.0))
              (Variables|Default|SetCurrentFuelTime (.FuelTime (Utilities|Struct|BreakS_FurnaceFuel (Variables|Default|GetFuel))))
              (if (<= (- (Utilities|Struct|BreakInventorySlot (Utilities|Array|Get(acopy) (Variables|/Game/Blueprints/Inventory.Inventory_C|GetSlots (Variables|Default|GetInventory_Fuel)))) (Utilities|Struct|BreakInventorySlot (.Fuel (Utilities|Struct|BreakS_FurnaceFuel (Variables|Default|GetFuel))))) 0)
                (Default|ServerSAEInventory _inventory_fuel)
                (else
                  (Default|ServerSAEInventory _inventory_fuel 0 (Utilities|Struct|MakeInventorySlot (.da_item _output) (- (Utilities|Struct|BreakInventorySlot (Utilities|Array|Get(acopy) (Variables|/Game/Blueprints/Inventory.Inventory_C|GetSlots (Variables|Default|GetInventory_Fuel)))) (Utilities|Struct|BreakInventorySlot (.Fuel (Utilities|Struct|BreakS_FurnaceFuel (Variables|Default|GetFuel))))) (.properties _output)))))))
          (:then_1
            (Variables|Default|SetFuelEfficiency (.FuelEfficiency (Utilities|Struct|BreakS_FurnaceFuel (Variables|Default|GetFuel))))
            (Variables|Default|SetMaxFuelTime (.FuelTime (Utilities|Struct|BreakS_FurnaceFuel (Variables|Default|GetFuel))))
            (Variables|Default|SetEndCookTime (.CookTime (Utilities|Struct|BreakS_FurnaceOutput (Variables|Default|GetOutput))))))
        (else
          (return))))))

(fn SavePlacedObject
  (bind _defaultsceneroot (Variables|Default|GetDefaultSceneRoot))
  (return (Utilities|Struct|MakeSW_PlacedObject (Utilities|Array|MakeArray (Variables|/Script/Engine.SceneComponent|GetRelativeLocation _defaultsceneroot)) (Utilities|Array|MakeArray (Variables|/Script/Engine.SceneComponent|GetRelativeRotation _defaultsceneroot)) (Utilities|Array|MakeArray (Utilities|Struct|MakeArrayInventorySlots (Variables|/Game/Blueprints/Inventory.Inventory_C|GetSlots (Variables|Default|GetInventory_Input))) (Utilities|Struct|MakeArrayInventorySlots (Variables|/Game/Blueprints/Inventory.Inventory_C|GetSlots (Variables|Default|GetInventory_Output))) (Utilities|Struct|MakeArrayInventorySlots (Variables|/Game/Blueprints/Inventory.Inventory_C|GetSlots (Variables|Default|GetInventory_Fuel)))))))

(fn LoadPlacedObject
  (params (SW_PlacedObject :type SW%20Placed%20Object%20Structure))
  (bind (_vectors _rotations _arrayinventoryslots) (Utilities|Struct|BreakSW_PlacedObject SW_PlacedObject))
  (Transformation|SetRelativeLocationAndRotation (Variables|Default|GetDefaultSceneRoot) (Utilities|Array|Get(acopy) _vectors) (Utilities|Array|Get(acopy) _rotations) false true)
  (for (_array_element _array_index) _arrayinventoryslots
    (Variables|/Game/Blueprints/Inventory.Inventory_C|SetSlots (Utilities|Select :Index _array_index :Option%200 (Variables|Default|GetInventory_Input) :Option%201 (Variables|Default|GetInventory_Output) :Option%202 (Variables|Default|GetInventory_Fuel)) (Utilities|Struct|BreakArrayInventorySlots _array_element))
    (return false)))

(fn ClientInteractBP
  (params (InteractKey :type EInteractKey%20Enum :default "Interact1") (Pawn :type Pawn%20Object%20Reference) (BP_PAI :type BP%20PAI%20Object%20Reference))
  (switch Utilities|FlowControl|Switch|SwitchonEInteractKey InteractKey
    (:Interact1
      (bind _returnvalue (UserInterface|CreateWidget "/Game/Widgets/CWS/CWS_Furnace.CWS_Furnace_C" 0 self Pawn))
      (UserInterface|Viewport|AddtoViewport _returnvalue 0)
      (Default|AddCWS BP_PAI _returnvalue true true "NewEnumerator2")
      (Default|SetMousetoCenter BP_PAI)
      (return true))))

(fn ClientInterruptBP
  (params (InterruptedBy :type EInterruptedBy%20Enum :default "Player") (InteractKey :type EInteractKey%20Enum :default "Interact1") (Pawn :type Pawn%20Object%20Reference) (BP_PAI :type BP%20PAI%20Object%20Reference))
  (return false))

(fn GetInteractLocation
  (return (Transformation|GetActorLocation)))

(fn GetInteractSystem
  (return (Variables|Default|GetInteractSystem)))

(fn ServerInteractBP
  (params (InteractKey :type EInteractKey%20Enum :default "Interact1") (Pawn :type Pawn%20Object%20Reference) (BP_PAI :type BP%20PAI%20Object%20Reference))
  (switch Utilities|FlowControl|Switch|SwitchonEInteractKey InteractKey
    (:Interact3
      (bind _inventory (Class|BPIGetInventory|GetInventory(Message) Pawn))
      (bind _success (Default|AddtoInventory _inventory (Variables|Default|GetFurnaceItem)))
      (if _success
        (Actor|DestroyActor)
        (return true)))))

(fn ServerInterruptBP
  (params (InterruptedBy :type EInterruptedBy%20Enum :default "Player") (InteractKey :type EInteractKey%20Enum :default "Interact1") (Pawn :type Pawn%20Object%20Reference) (BP_PAI :type BP%20PAI%20Object%20Reference))
  (return false))