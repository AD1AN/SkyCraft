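; AstralCore is an interactable that gives an astral character access to the Astralons screen and a way to leave the Astral.
; Client interaction requires a CharAstral pawn: the first interact option creates the CWS_Astralons widget with the character and Island, registers it with BPPSS and centers the mouse.
; The second option calls LeaveAstral on BPPSS.
; Server interaction and both interrupt handlers contain no behavior.
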(fn ConstructionScript)

(fn ClientInteractBP
  (params (InteractKey :type EInteractKey%20Enum :default "Interact1") (Pawn :type Pawn%20Object%20Reference) (BP_PSS :type BP%20PSS%20Object%20Reference))
  (bind _aschar_astral (Utilities|Casting|CastToCharAstral Pawn))
  (LocalVariables|Set_CharAstral _aschar_astral)
  (switch Utilities|FlowControl|Switch|SwitchonEInteractKey InteractKey
    (:Interact1
      (bind _returnvalue (UserInterface|CreateWidget "/Game/Widgets/CWS/CWS_Astralons.CWS_Astralons_C" 0 (LocalVariables|Get_CharAstral) (Variables|/Game/Blueprints/Astral.Astral_C|GetIsland (Variables|Default|GetAstral))))
      (UserInterface|Viewport|AddtoViewport _returnvalue 10)
      (Default|AddCWS BP_PSS _returnvalue true true true "NewEnumerator2")
      (Default|SetMousetoCenter BP_PSS))
    (:Interact2
      (Default|LeaveAstral BP_PSS (LocalVariables|Get_CharAstral)))))

(fn ClientInterruptBP
  (params (InterruptedBy :type EInterruptedBy%20Enum :default "Player") (InteractKey :type EInteractKey%20Enum :default "Interact1") (Pawn :type Pawn%20Object%20Reference) (BP_PSS :type BP%20PSS%20Object%20Reference))
  (return false))

(fn ServerInteractBP
  (params (InteractKey :type EInteractKey%20Enum :default "Interact1") (Pawn :type Pawn%20Object%20Reference) (BP_PSS :type BP%20PSS%20Object%20Reference))
  (switch Utilities|FlowControl|Switch|SwitchonEInteractKey InteractKey))

(fn ServerInterruptBP
  (params (InterruptedBy :type EInterruptedBy%20Enum :default "Player") (InteractKey :type EInteractKey%20Enum :default "Interact1") (Pawn :type Pawn%20Object%20Reference) (BP_PSS :type BP%20PSS%20Object%20Reference))
  (return false))