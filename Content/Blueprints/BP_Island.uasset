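; BP_Island is a generated island actor whose server picks a seeded random biome and populates it.
; On generation and chunk LOD changes, it works from the farthest unprocessed LOD down to the chunk's current one.
; Saved islands restore LODs through EntityGenerator, plus buildings and dropped items at LOD 0.
; Remaining LODs get probability-weighted resources and NPCs from the biome data asset; destruction clears them all.
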(event Custom|OnChangeLOD_Event
  (bind _ss_island (Variables|Default|GetSS_Island))
  (bind _da_islandbiome (Variables|Default|GetDA_IslandBiome))
  (bind _islandlods (Variables|/Script/SkyCraft.DA_IslandBiome|GetIslandLODs _da_islandbiome))
  (if (< (Variables|/Game/Blueprints/BP_ChunkIsland.BP_ChunkIsland_C|GetCurrentLOD (Variables|Default|GetChunk)) (Variables|Default|GetLastLOD))
    (if (Variables|Default|GetbIslandFromSave)
      (Variables|Default|SetLoadedLowestLOD (Variables|Default|GetLastLOD))
      (Variables|Default|Set_IndexSubtract 0)
      (for _index (range (Variables|/Game/Blueprints/BP_ChunkIsland.BP_ChunkIsland_C|GetCurrentLOD (Variables|Default|GetChunk)) (- (Variables|Default|GetLastLOD) 1))
        (if (== (- (- (Variables|Default|GetLastLOD) 1) (Variables|Default|Get_IndexSubtract)) 0)
          (Default|LoadBuildings (Variables|/Game/Blueprints/BP_GSS.BP_GSS_C|GetBP_GMS (Variables|Default|GetBP_GSS)) (.buildings _ss_island) self)
          (Class|Island|LoadDroppedItems (.droppeditems _ss_island)))
        (bind _returnvalue (Class|EntityGenerator|LoadLOD (Variables|Default|GetEntityGenerator) (.islandlods _ss_island) (- (- (Variables|Default|GetLastLOD) 1) (Variables|Default|Get_IndexSubtract))))
        (if _returnvalue
          (Variables|Default|SetLoadedLowestLOD (Math|Integer|Min(Integer) (- (- (Variables|Default|GetLastLOD) 1) (Variables|Default|Get_IndexSubtract)) (Variables|Default|GetLastLOD))))
        (Math|Integer|IncrementInt (Variables|Default|Get_IndexSubtract)))
      (Variables|Default|SetLastLOD (Variables|Default|GetLoadedLowestLOD)))
    (Variables|Default|Set_IndexSubtract 0)
    (for _index_2 (range (Variables|/Game/Blueprints/BP_ChunkIsland.BP_ChunkIsland_C|GetCurrentLOD (Variables|Default|GetChunk)) (- (Variables|Default|GetLastLOD) 1))
      (if (Utilities|Array|IsValidIndex _islandlods (- (- (Variables|Default|GetLastLOD) 1) (Variables|Default|Get_IndexSubtract)))
        (for _array_element (.Resources (Utilities|Struct|BreakIslandLOD (Utilities|Array|Get(acopy) _islandlods (- (- (Variables|Default|GetLastLOD) 1) (Variables|Default|Get_IndexSubtract)))))
          (if (Math|Random|RandomBoolwithWeight (.Probability (Utilities|Struct|BreakIslandResource _array_element)))
            (Class|EntityGenerator|GenerateResources (Variables|Default|GetEntityGenerator) (Utilities|Struct|MakeGenerateResourcesIn (.MaxSpawnPoints (Utilities|Struct|BreakIslandResource _array_element)) (.DA_Resource (Utilities|Struct|BreakIslandResource _array_element)) (.ResourceSize (Utilities|Struct|BreakIslandResource _array_element)) (- (- (Variables|Default|GetLastLOD) 1) (Variables|Default|Get_IndexSubtract))))))
        (for _array_element_2 (.NPCs (Utilities|Struct|BreakIslandLOD (Utilities|Array|Get(acopy) _islandlods (- (- (Variables|Default|GetLastLOD) 1) (Variables|Default|Get_IndexSubtract)))))
          (if (Math|Random|RandomBoolwithWeight (.Probability (Utilities|Struct|BreakIslandNPC _array_element_2)))
            (Class|EntityGenerator|GenerateNPCs (Variables|Default|GetEntityGenerator) (Utilities|Struct|MakeGenerateNPCsIn (.MaxSpawnPoints (Utilities|Struct|BreakIslandNPC _array_element_2)) (.NPC_Class (Utilities|Struct|BreakIslandNPC _array_element_2)) 8e+01 (- (- (Variables|Default|GetLastLOD) 1) (Variables|Default|Get_IndexSubtract))))))
        (Math|Integer|IncrementInt (Variables|Default|Get_IndexSubtract))))
    (Variables|Default|SetLastLOD (Variables|/Game/Blueprints/BP_ChunkIsland.BP_ChunkIsland_C|GetCurrentLOD (Variables|Default|GetChunk)))
    (Variables|Default|SetbIslandCanSave true)))

(event Custom|OnGenerated_Event
  (params (Island :type Island%20Object%20Reference))
  (bind _ss_island (Variables|Default|GetSS_Island))
  (bind _da_islandbiome (Variables|Default|GetDA_IslandBiome))
  (bind _islandlods (Variables|/Script/SkyCraft.DA_IslandBiome|GetIslandLODs _da_islandbiome))
  (Variables|Default|SetLastLOD (Math|Integer|Max(Integer) (Variables|/Script/SkyCraft.GSS|GetChunkRenderRange (Variables|Default|GetBP_GSS)) (Utilities|Array|Length (Variables|/Script/SkyCraft.DA_IslandBiome|GetIslandLODs (Variables|Default|GetDA_IslandBiome)))))
  (EventDispatchers|BindEventtoOnChangeLOD (Variables|Default|GetChunk) (delegate Custom|OnChangeLOD_Event))
  (if (< (Variables|/Game/Blueprints/BP_ChunkIsland.BP_ChunkIsland_C|GetCurrentLOD (Variables|Default|GetChunk)) (Variables|Default|GetLastLOD))
    (if (Variables|Default|GetbIslandFromSave)
      (Variables|Default|SetLoadedLowestLOD (Variables|Default|GetLastLOD))
      (Variables|Default|Set_IndexSubtract 0)
      (for _index (range (Variables|/Game/Blueprints/BP_ChunkIsland.BP_ChunkIsland_C|GetCurrentLOD (Variables|Default|GetChunk)) (- (Variables|Default|GetLastLOD) 1))
        (if (== (- (- (Variables|Default|GetLastLOD) 1) (Variables|Default|Get_IndexSubtract)) 0)
          (Default|LoadBuildings (Variables|/Game/Blueprints/BP_GSS.BP_GSS_C|GetBP_GMS (Variables|Default|GetBP_GSS)) (.buildings _ss_island) self)
          (Class|Island|LoadDroppedItems (.droppeditems _ss_island)))
        (bind _returnvalue (Class|EntityGenerator|LoadLOD (Variables|Default|GetEntityGenerator) (.islandlods _ss_island) (- (- (Variables|Default|GetLastLOD) 1) (Variables|Default|Get_IndexSubtract))))
        (if _returnvalue
          (Variables|Default|SetLoadedLowestLOD (Math|Integer|Min(Integer) (- (- (Variables|Default|GetLastLOD) 1) (Variables|Default|Get_IndexSubtract)) (Variables|Default|GetLastLOD))))
        (Math|Integer|IncrementInt (Variables|Default|Get_IndexSubtract)))
      (Variables|Default|SetLastLOD (Variables|Default|GetLoadedLowestLOD)))
    (Variables|Default|Set_IndexSubtract 0)
    (for _index_2 (range (Variables|/Game/Blueprints/BP_ChunkIsland.BP_ChunkIsland_C|GetCurrentLOD (Variables|Default|GetChunk)) (- (Variables|Default|GetLastLOD) 1))
      (if (Utilities|Array|IsValidIndex _islandlods (- (- (Variables|Default|GetLastLOD) 1) (Variables|Default|Get_IndexSubtract)))
        (for _array_element (.Resources (Utilities|Struct|BreakIslandLOD (Utilities|Array|Get(acopy) _islandlods (- (- (Variables|Default|GetLastLOD) 1) (Variables|Default|Get_IndexSubtract)))))
          (if (Math|Random|RandomBoolwithWeight (.Probability (Utilities|Struct|BreakIslandResource _array_element)))
            (Class|EntityGenerator|GenerateResources (Variables|Default|GetEntityGenerator) (Utilities|Struct|MakeGenerateResourcesIn (.MaxSpawnPoints (Utilities|Struct|BreakIslandResource _array_element)) (.DA_Resource (Utilities|Struct|BreakIslandResource _array_element)) (.ResourceSize (Utilities|Struct|BreakIslandResource _array_element)) (- (- (Variables|Default|GetLastLOD) 1) (Variables|Default|Get_IndexSubtract))))))
        (for _array_element_2 (.NPCs (Utilities|Struct|BreakIslandLOD (Utilities|Array|Get(acopy) _islandlods (- (- (Variables|Default|GetLastLOD) 1) (Variables|Default|Get_IndexSubtract)))))
          (if (Math|Random|RandomBoolwithWeight (.Probability (Utilities|Struct|BreakIslandNPC _array_element_2)))
            (Class|EntityGenerator|GenerateNPCs (Variables|Default|GetEntityGenerator) (Utilities|Struct|MakeGenerateNPCsIn (.MaxSpawnPoints (Utilities|Struct|BreakIslandNPC _array_element_2)) (.NPC_Class (Utilities|Struct|BreakIslandNPC _array_element_2)) 8e+01 (- (- (Variables|Default|GetLastLOD) 1) (Variables|Default|Get_IndexSubtract))))))
        (Math|Integer|IncrementInt (Variables|Default|Get_IndexSubtract))))
    (Variables|Default|SetLastLOD (Variables|/Game/Blueprints/BP_ChunkIsland.BP_ChunkIsland_C|GetCurrentLOD (Variables|Default|GetChunk)))
    (Variables|Default|SetbIslandCanSave true)))

(event EventBeginPlay
  (Networking|SwitchHasAuthority
    (:Authority
      (EventDispatchers|BindEventtoOnIslandGenerated (delegate Custom|OnGenerated_Event))
      (Variables|Default|SetDA_IslandBiome (.OutItem (Utilities|Array|RandomFromStream (Variables|/Game/Blueprints/BP_GMS.BP_GMS_C|GetDA_IslandBiomes (Variables|/Game/Blueprints/BP_GSS.BP_GSS_C|GetBP_GMS (Variables|Default|GetBP_GSS))) (Variables|Default|GetSeed)))))))

(event EventDestroyed
  (Networking|SwitchHasAuthority
    (:Authority
      (Class|EntityGenerator|DestroyLODs (Variables|Default|GetEntityGenerator)))))

(fn ConstructionScript)