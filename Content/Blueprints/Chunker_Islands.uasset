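; Server-side component that streams floating island chunks in a circular grid range around its owner.
; On a roughly one-second tick, a cell change makes it unregister from distant chunks, then reuse or spawn chunks through a shared BPGMS registry.
; New chunks derive seed and size from coordinates plus world seed, then probabilistically spawn an island, restoring saved data if present.
; TransferChunks copies tracking state from another generator.
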(event EventEndPlay
  (params (EndPlayReason :type EEndPlayReason%20Enum :default "Destroyed"))
  (Networking|SwitchHasAuthority
    (:Authority
      (for _array_element (Variables|Default|GetRenderingChunks)
        (Default|RemoveGenerator _array_element self)))))

(event EventTick
  (params (DeltaSeconds :type Float%20%28single-precision%29))
  (CallFunction|CheckChunk))

(event EventBeginPlay
  (Networking|SwitchHasAuthority
    (:Authority
      (bind _asbp_gss (Utilities|Casting|CastToBP_GSS (Game|GetGameState)))
      (Variables|Default|SetBP_GSS _asbp_gss)
      (if (Class|LowEntryExtendedStandardLibrary|ShippingBuild)
        _
        (else
          ;[0.5104 0 0] Debug
          (bind _asbp_gis (Utilities|Casting|CastToBP_GIS (Game|GetGameInstance)))
          (if (Variables|/Game/Blueprints/BP_GIS.BP_GIS_C|GetisTestChunkIslandRenderRange _asbp_gis)
            (Variables|/Script/SkyCraft.GSS|SetChunkRenderRange (Variables|Default|GetBP_GSS) (Variables|/Game/Blueprints/BP_GIS.BP_GIS_C|GetTestChunkIslandRenderRange _asbp_gis)))))
      (Class|ActorComponent|SetComponentTickInterval (Math|Random|RandomFloatinRange 0.9 1.0))
      (Components|Tick|SetComponentTickEnabled true)
      (CallFunction|CheckChunk))))

(fn CheckChunk
  (bind _output_get (Variables|Default|SetCurrentCoords (CallFunction|GetCoords)))
  (if (not (and (== (.x _output_get) (.x (Variables|Default|GetPreviousCoords))) (== (.y _output_get) (.y (Variables|Default|GetPreviousCoords)))))
    (Variables|Default|SetPreviousCoords (Variables|Default|GetCurrentCoords))
    (CallFunction|DestroyChunks)
    (CallFunction|SpawnChunks)))

(fn GetCoords
  (bind _returnvalue (Components|GetOwner))
  (bind _bp_gss (Variables|Default|GetBP_GSS))
  (bind _returnvalue_2 (Transformation|GetActorLocation _returnvalue))
  (bind _chunksize (Variables|/Script/SkyCraft.GSS|GetChunkSize _bp_gss))
  (bind _returnvalue_3 (/ _returnvalue_2 _chunksize))
  (bind (_x _y) (Math|Vector|BreakVector _returnvalue_3))
  (return (Utilities|Struct|MakeInt2Vector (Math|Float|Round _x) (Math|Float|Round _y))))

(fn DestroyChunks
  (bind _currentcoords (Variables|Default|GetCurrentCoords))
  (bind _bp_gss (Variables|Default|GetBP_GSS))
  (bind _bp_gss_2 (Variables|Default|GetBP_GSS))
  (bind _bp_gss_3 (Variables|Default|GetBP_GSS))
  (bind _chunksize (Variables|/Script/SkyCraft.GSS|GetChunkSize _bp_gss_2))
  (bind _chunksize_2 (Variables|/Script/SkyCraft.GSS|GetChunkSize _bp_gss_3))
  (bind (_arrayindex _arrayelement) (Utilities|Array|ReverseforEachLoop (Variables|Default|GetRenderingCoords))
    (:LoopBody
      (LocalVariables|Set_IndexCoords _arrayindex)
      (if (>= (Math|Vector|Distance(Vector) (Math|Vector|MakeVector (* (.X (Utilities|Struct|BreakInt2Vector _arrayelement)) _chunksize) (* (.Y (Utilities|Struct|BreakInt2Vector _arrayelement)) _chunksize) 0.0) (Math|Vector|MakeVector (* (.x _currentcoords) _chunksize_2) (* (.y _currentcoords) _chunksize_2) 0.0)) (* (Variables|/Script/SkyCraft.GSS|GetChunkRenderRange _bp_gss) (Variables|/Script/SkyCraft.GSS|GetChunkSize _bp_gss)))
        (Default|RemoveGenerator (Utilities|Array|Get(acopy) (Variables|Default|GetRenderingChunks) (LocalVariables|Get_IndexCoords)) self)
        (Utilities|Array|RemoveIndex (Variables|Default|GetRenderingCoords) (LocalVariables|Get_IndexCoords))
        (Utilities|Array|RemoveIndex (Variables|Default|GetRenderingChunks) (LocalVariables|Get_IndexCoords))))))

(fn SpawnChunks
  (bind _returnvalue (Class|KismetSystemLibrary|MakeLiteralInteger 200))
  (bind _returnvalue_2 (Class|KismetSystemLibrary|MakeLiteralInteger 50))
  (bind _bp_gss (Variables|Default|GetBP_GSS))
  (bind _currentcoords (Variables|Default|GetCurrentCoords))
  (bind _bp_gss_2 (Variables|Default|GetBP_GSS))
  (bind _bp_gss_3 (Variables|Default|GetBP_GSS))
  (bind _bp_gss_4 (Variables|Default|GetBP_GSS))
  (bind _bp_gss_5 (Variables|Default|GetBP_GSS))
  (bind _bp_gss_6 (Variables|Default|GetBP_GSS))
  (bind _bp_gss_7 (Variables|Default|GetBP_GSS))
  (bind _bp_gss_8 (Variables|Default|GetBP_GSS))
  (bind _chunksize (Variables|/Script/SkyCraft.GSS|GetChunkSize _bp_gss))
  (bind _chunkrenderrange (Variables|/Script/SkyCraft.GSS|GetChunkRenderRange _bp_gss_2))
  (bind _chunkrenderrange_2 (Variables|/Script/SkyCraft.GSS|GetChunkRenderRange _bp_gss_5))
  (bind _chunksize_2 (Variables|/Script/SkyCraft.GSS|GetChunkSize _bp_gss_3))
  (bind _islandsaltitude (Variables|/Script/SkyCraft.GSS|GetIslandsAltitude _bp_gss_8))
  (bind _bp_gms (Variables|/Game/Blueprints/BP_GSS.BP_GSS_C|GetBP_GMS _bp_gss_6))
  (bind _bp_gms_2 (Variables|/Game/Blueprints/BP_GSS.BP_GSS_C|GetBP_GMS _bp_gss_7))
  (for _index (range (* _chunkrenderrange -1) _chunkrenderrange)
    (LocalVariables|Set_LocalX _index)
    (for _index_2 (range (* _chunkrenderrange_2 -1) _chunkrenderrange_2)
      (LocalVariables|Set_LocalY _index_2)
      (LocalVariables|Set_ChunkWorldCoords (Utilities|Struct|MakeInt2Vector (+ (.x _currentcoords) (LocalVariables|Get_LocalX)) (+ (.y _currentcoords) (LocalVariables|Get_LocalY))))
      (if (< (Math|Vector|VectorLength (Math|Vector|MakeVector (* (LocalVariables|Get_LocalX) _chunksize) (* (LocalVariables|Get_LocalY) _chunksize) 0.0)) (* (Variables|/Script/SkyCraft.GSS|GetChunkRenderRange _bp_gss_4) (Variables|/Script/SkyCraft.GSS|GetChunkSize _bp_gss_4)))
        (if (>= (Utilities|Array|FindItem (Variables|Default|GetRenderingCoords) (LocalVariables|Get_ChunkWorldCoords)) 0)
          (Default|UpdateLOD (Utilities|Array|Get(acopy) (Variables|Default|GetRenderingChunks) (Utilities|Array|FindItem (Variables|Default|GetRenderingCoords) (LocalVariables|Get_ChunkWorldCoords))))
          (elif (Utilities|Array|ContainsItem (Variables|/Game/Blueprints/BP_GMS.BP_GMS_C|GetSpawnedChunkIslandsCors (Variables|/Game/Blueprints/BP_GSS.BP_GSS_C|GetBP_GMS (Variables|Default|GetBP_GSS))) (LocalVariables|Get_ChunkWorldCoords))
            (Utilities|Array|Add (Variables|Default|GetRenderingCoords) (LocalVariables|Get_ChunkWorldCoords))
            (Utilities|Array|Add (Variables|Default|GetRenderingChunks) (Utilities|Array|Get(acopy) (Variables|/Game/Blueprints/BP_GMS.BP_GMS_C|GetSpawnedChunkIslands _bp_gms) (Utilities|Array|FindItem (Variables|/Game/Blueprints/BP_GMS.BP_GMS_C|GetSpawnedChunkIslandsCors _bp_gms) (LocalVariables|Get_ChunkWorldCoords))))
            (Default|AddGenerator (Utilities|Array|Get(acopy) (Variables|/Game/Blueprints/BP_GMS.BP_GMS_C|GetSpawnedChunkIslands _bp_gms) (Utilities|Array|FindItem (Variables|/Game/Blueprints/BP_GMS.BP_GMS_C|GetSpawnedChunkIslandsCors _bp_gms) (LocalVariables|Get_ChunkWorldCoords))) self)
            (else
              (bind _returnvalue_3 (Game|SpawnActorfromClass "/Game/Blueprints/BP_ChunkIsland.BP_ChunkIsland_C" (Math|Transform|MakeTransform (Math|Vector|MakeVector (* (.x (LocalVariables|Get_ChunkWorldCoords)) _chunksize_2) (* (.y (LocalVariables|Get_ChunkWorldCoords)) _chunksize_2) 5e+04) "0, 0, 0" "1.000000,1.000000,1.000000") "AlwaysSpawn" "OverrideRootScale" 0 (Variables|/Game/Blueprints/BP_GSS.BP_GSS_C|GetBP_GMS (Variables|Default|GetBP_GSS)) (LocalVariables|Get_ChunkWorldCoords) (CallFunction|Int->Stream->Int (+ (CallFunction|Int->Stream->Int (.x (LocalVariables|Get_ChunkWorldCoords))) (.y (LocalVariables|Get_ChunkWorldCoords)) (Variables|/Game/Blueprints/BP_GMS.BP_GMS_C|GetWorldSeed (Variables|/Game/Blueprints/BP_GSS.BP_GSS_C|GetBP_GMS (Variables|Default|GetBP_GSS))))) (Math|Random|RandomIntegerinRangefromStream (Math|Random|MakeRandomStream (CallFunction|Int->Stream->Int (+ (CallFunction|Int->Stream->Int (.x (LocalVariables|Get_ChunkWorldCoords))) (.y (LocalVariables|Get_ChunkWorldCoords)) (Variables|/Game/Blueprints/BP_GMS.BP_GMS_C|GetWorldSeed (Variables|/Game/Blueprints/BP_GSS.BP_GSS_C|GetBP_GMS (Variables|Default|GetBP_GSS)))))) _returnvalue_2 _returnvalue) (Math|Float|MapRangeClamped (Math|Conversions|ToFloat(Integer) (Math|Random|RandomIntegerinRangefromStream (Math|Random|MakeRandomStream (CallFunction|Int->Stream->Int (+ (CallFunction|Int->Stream->Int (.x (LocalVariables|Get_ChunkWorldCoords))) (.y (LocalVariables|Get_ChunkWorldCoords)) (Variables|/Game/Blueprints/BP_GMS.BP_GMS_C|GetWorldSeed (Variables|/Game/Blueprints/BP_GSS.BP_GSS_C|GetBP_GMS (Variables|Default|GetBP_GSS)))))) _returnvalue_2 _returnvalue)) (Math|Conversions|ToFloat(Integer) _returnvalue_2) (Math|Conversions|ToFloat(Integer) _returnvalue) 0.0 1.0) (Utilities|Array|MakeArray self) 0))
              (LocalVariables|Set_SpawnedChunk _returnvalue_3)
              (Utilities|FlowControl|Sequence
                (:then_0
                  (Utilities|Array|Add (Variables|/Game/Blueprints/BP_GMS.BP_GMS_C|GetSpawnedChunkIslands _bp_gms_2) (LocalVariables|Get_SpawnedChunk))
                  (Utilities|Array|Add (Variables|/Game/Blueprints/BP_GMS.BP_GMS_C|GetSpawnedChunkIslandsCors _bp_gms_2) (LocalVariables|Get_ChunkWorldCoords))
                  (Utilities|Array|Add (Variables|Default|GetRenderingChunks) (LocalVariables|Get_SpawnedChunk))
                  (Utilities|Array|Add (Variables|Default|GetRenderingCoords) (LocalVariables|Get_ChunkWorldCoords)))
                (:then_1
                  (if (Class|KismetMathLibrary|RandomBoolwithWeightfromStream (Math|Random|MakeRandomStream (CallFunction|Int->Stream->Int (CallFunction|Int->Stream->Int (+ (CallFunction|Int->Stream->Int (.x (LocalVariables|Get_ChunkWorldCoords))) (.y (LocalVariables|Get_ChunkWorldCoords)) (Variables|/Game/Blueprints/BP_GMS.BP_GMS_C|GetWorldSeed (Variables|/Game/Blueprints/BP_GSS.BP_GSS_C|GetBP_GMS (Variables|Default|GetBP_GSS))))))) (Variables|Default|GetIslandsProbabilityWeight))
                    (if (.ReturnValue (Utilities|Map|Find (Variables|/Game/Blueprints/BP_GMS.BP_GMS_C|GetSavedIslandStatics (Variables|/Game/Blueprints/BP_GSS.BP_GSS_C|GetBP_GMS (Variables|Default|GetBP_GSS))) (LocalVariables|Get_ChunkWorldCoords)))
                      (bind _returnvalue_4 (Game|SpawnActorfromClass "/Game/Blueprints/IslandStatic.IslandStatic_C" (Math|Transform|MakeTransform (Math|Vector|MakeVector (.x (Transformation|GetActorLocation (LocalVariables|Get_SpawnedChunk))) (.y (Transformation|GetActorLocation (LocalVariables|Get_SpawnedChunk))) (+ (.z (Transformation|GetActorLocation (LocalVariables|Get_SpawnedChunk))) (Math|Random|RandomFloatinRangefromStream (Math|Random|MakeRandomStream (Variables|/Game/Blueprints/BP_ChunkIsland.BP_ChunkIsland_C|GetSeed (LocalVariables|Get_SpawnedChunk))) (.min _islandsaltitude) (.max _islandsaltitude)))) "0, 0, 0" "1.000000,1.000000,1.000000") "AlwaysSpawn" "MultiplyWithRoot" 0 (Variables|Default|GetBP_GSS) (LocalVariables|Get_SpawnedChunk) (LocalVariables|Get_ChunkWorldCoords) true (.Value (Utilities|Map|Find (Variables|/Game/Blueprints/BP_GMS.BP_GMS_C|GetSavedIslandStatics (Variables|/Game/Blueprints/BP_GSS.BP_GSS_C|GetBP_GMS (Variables|Default|GetBP_GSS))) (LocalVariables|Get_ChunkWorldCoords))) (Variables|/Game/Blueprints/BP_ChunkIsland.BP_ChunkIsland_C|GetSeed (LocalVariables|Get_SpawnedChunk)) (Math|Float|MapRangeClamped (Math|Conversions|ToFloat(Integer) (Math|Random|RandomIntegerinRangefromStream (Math|Random|MakeRandomStream (CallFunction|Int->Stream->Int (+ (CallFunction|Int->Stream->Int (.x (LocalVariables|Get_ChunkWorldCoords))) (.y (LocalVariables|Get_ChunkWorldCoords)) (Variables|/Game/Blueprints/BP_GMS.BP_GMS_C|GetWorldSeed (Variables|/Game/Blueprints/BP_GSS.BP_GSS_C|GetBP_GMS (Variables|Default|GetBP_GSS)))))) _returnvalue_2 _returnvalue)) (Math|Conversions|ToFloat(Integer) _returnvalue_2) (Math|Conversions|ToFloat(Integer) _returnvalue) 0.0 1.0) (Math|Random|RandomIntegerinRangefromStream (Math|Random|MakeRandomStream (CallFunction|Int->Stream->Int (+ (CallFunction|Int->Stream->Int (.x (LocalVariables|Get_ChunkWorldCoords))) (.y (LocalVariables|Get_ChunkWorldCoords)) (Variables|/Game/Blueprints/BP_GMS.BP_GMS_C|GetWorldSeed (Variables|/Game/Blueprints/BP_GSS.BP_GSS_C|GetBP_GMS (Variables|Default|GetBP_GSS)))))) _returnvalue_2 _returnvalue) 0))
                      (Variables|/Game/Blueprints/BP_ChunkIsland.BP_ChunkIsland_C|SetIslandStatic (LocalVariables|Get_SpawnedChunk) _returnvalue_4)
                      (Variables|/Game/Blueprints/IslandStatic.IslandStatic_C|SetChunk _returnvalue_4 (LocalVariables|Get_SpawnedChunk))
                      (else
                        (bind _returnvalue_5 (Game|SpawnActorfromClass :Class "/Game/Blueprints/IslandStatic.IslandStatic_C" :SpawnTransform (Math|Transform|MakeTransform (Math|Vector|MakeVector (.x (Transformation|GetActorLocation (LocalVariables|Get_SpawnedChunk))) (.y (Transformation|GetActorLocation (LocalVariables|Get_SpawnedChunk))) (+ (.z (Transformation|GetActorLocation (LocalVariables|Get_SpawnedChunk))) (Math|Random|RandomFloatinRangefromStream (Math|Random|MakeRandomStream (Variables|/Game/Blueprints/BP_ChunkIsland.BP_ChunkIsland_C|GetSeed (LocalVariables|Get_SpawnedChunk))) (.min _islandsaltitude) (.max _islandsaltitude)))) "0, 0, 0" "1.000000,1.000000,1.000000") :CollisionHandlingOverride "AlwaysSpawn" :TransformScaleMethod "MultiplyWithRoot" :BP_GSS (Variables|Default|GetBP_GSS) :Chunk (LocalVariables|Get_SpawnedChunk) :ChunkCoords (LocalVariables|Get_ChunkWorldCoords) :Seed (Variables|/Game/Blueprints/BP_ChunkIsland.BP_ChunkIsland_C|GetSeed (LocalVariables|Get_SpawnedChunk)) :IslandSizeRatio (Math|Float|MapRangeClamped (Math|Conversions|ToFloat(Integer) (Math|Random|RandomIntegerinRangefromStream (Math|Random|MakeRandomStream (CallFunction|Int->Stream->Int (+ (CallFunction|Int->Stream->Int (.x (LocalVariables|Get_ChunkWorldCoords))) (.y (LocalVariables|Get_ChunkWorldCoords)) (Variables|/Game/Blueprints/BP_GMS.BP_GMS_C|GetWorldSeed (Variables|/Game/Blueprints/BP_GSS.BP_GSS_C|GetBP_GMS (Variables|Default|GetBP_GSS)))))) _returnvalue_2 _returnvalue)) (Math|Conversions|ToFloat(Integer) _returnvalue_2) (Math|Conversions|ToFloat(Integer) _returnvalue) 0.0 1.0) :IslandSize (Math|Random|RandomIntegerinRangefromStream (Math|Random|MakeRandomStream (CallFunction|Int->Stream->Int (+ (CallFunction|Int->Stream->Int (.x (LocalVariables|Get_ChunkWorldCoords))) (.y (LocalVariables|Get_ChunkWorldCoords)) (Variables|/Game/Blueprints/BP_GMS.BP_GMS_C|GetWorldSeed (Variables|/Game/Blueprints/BP_GSS.BP_GSS_C|GetBP_GMS (Variables|Default|GetBP_GSS)))))) _returnvalue_2 _returnvalue) :Instigator 0))
                        (Variables|/Game/Blueprints/BP_ChunkIsland.BP_ChunkIsland_C|SetIslandStatic (LocalVariables|Get_SpawnedChunk) _returnvalue_5)
                        (Variables|/Game/Blueprints/IslandStatic.IslandStatic_C|SetChunk _returnvalue_5 (LocalVariables|Get_SpawnedChunk))))))))))))))

(fn TransferChunks
  (params (FromGenerator :type Chunker%20Islands%20Object%20Reference))
  (Variables|Default|SetRenderingChunks (Variables|Chunker_Islands_C|GetRenderingChunks FromGenerator))
  (Variables|Default|SetRenderingCoords (Variables|Chunker_Islands_C|GetRenderingCoords FromGenerator))
  (Variables|Default|SetPreviousCoords (Variables|Chunker_Islands_C|GetPreviousCoords FromGenerator)))