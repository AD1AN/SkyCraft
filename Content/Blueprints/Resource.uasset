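; Resource is a harvestable world resource actor, either a Kark tree or stone, whose look and maximum health depend on its type and size.
; On BeginPlay it picks the static mesh by size, with stones also choosing between two varieties.
; It sets custom primitive data for material tuning per size, wind intensity for trees and texture scale for stones.
; The construction script is empty, so this setup only applies at runtime.
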(event EventBeginPlay
  (bind _resourcevariety (Variables|Default|GetResourceVariety))
  (switch Utilities|FlowControl|Switch|SwitchonE_ResourceType (Variables|Default|GetResourceType)
    (:NewEnumerator0
      (Components|StaticMesh|SetStaticMesh (Variables|Default|GetStaticMesh) (Utilities|Select :Index (Variables|Default|GetResourceSize) :Option%200 "/Game/Models/VEGETATION/KarkTree/KarkTree_small01.KarkTree_small01" :Option%201 "/Game/Models/VEGETATION/KarkTree/KarkTree_medium01.KarkTree_medium01" :Option%202 "/Game/Models/VEGETATION/KarkTree/KarkTree_big01.KarkTree_big01" :Option%203 "/Game/Models/VEGETATION/KarkTree/KarkTree_large01.KarkTree_large01"))
      (Rendering|Material|SetScalarParameterforCustomPrimitiveData (Variables|Default|GetStaticMesh) "WIntensity" (Utilities|Select :Index (Variables|Default|GetResourceSize) :Option%200 0.05 :Option%201 0.1 :Option%202 0.3 :Option%203 0.5))
      (Variables|Default|SetMaxHealth (Utilities|Select :Index (Variables|Default|GetResourceSize) :Option%200 1e+02 :Option%201 1.5e+02 :Option%202 2e+02 :Option%203 3e+02)))
    (:NewEnumerator1
      (Components|StaticMesh|SetStaticMesh (Variables|Default|GetStaticMesh) (Utilities|Select :Index (Variables|Default|GetResourceSize) :Option%200 (Utilities|Select :Index _resourcevariety :Option%200 "/Game/s2u/Stone_small1.Stone_small1" :Option%201 "/Game/s2u/Stone_small2.Stone_small2") :Option%201 (Utilities|Select :Index _resourcevariety :Option%200 "/Game/s2u/Stone_medium1.Stone_medium1" :Option%201 "/Game/s2u/Stone_medium2.Stone_medium2") :Option%202 (Utilities|Select :Index _resourcevariety :Option%200 "/Game/s2u/Stone_big1.Stone_big1" :Option%201 "/Game/s2u/Stone_big2.Stone_big2") :Option%203 (Utilities|Select :Index _resourcevariety :Option%200 "/Game/s2u/Stone_large1.Stone_large1" :Option%201 "/Game/s2u/Stone_large2.Stone_large2")))
      (Rendering|Material|SetScalarParameterforCustomPrimitiveData (Variables|Default|GetStaticMesh) "TextureScale" (Utilities|Select :Index (Variables|Default|GetResourceSize) :Option%200 3.0 :Option%201 3.5 :Option%202 4.0 :Option%203 5.0))
      (Variables|Default|SetMaxHealth (Utilities|Select :Index (Variables|Default|GetResourceSize) :Option%200 1e+02 :Option%201 1.5e+02 :Option%202 2e+02 :Option%203 3e+02)))))

(fn ConstructionScript)