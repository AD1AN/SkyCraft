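; Actor component that smoothly rotates its owning actor's yaw toward a target angle.
; StartYawInterp stores the target and speed, resets a timer and enables the component's tick.
; Each tick interpolates only yaw with RInterpTo, keeping pitch and roll.
; Tick switches itself off once yaw is within a small tolerance of the target, or after a safety timeout.
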(event EventTick
  (params (DeltaSeconds :type Float%20%28single-precision%29))
  (bind _returnvalue (Components|GetOwner))
  (bind _targetyaw (Variables|Default|GetTargetYaw))
  (bind _returnvalue_2 (Transformation|GetActorRotation _returnvalue))
  (Transformation|SetActorRotation _returnvalue (Math|Interpolation|RInterpTo (Math|Rotator|MakeRotator (.roll _returnvalue_2) (.pitch _returnvalue_2) (.yaw _returnvalue_2)) (Math|Rotator|MakeRotator (.roll _returnvalue_2) (.pitch _returnvalue_2) (Variables|Default|GetTargetYaw)) (Utilities|Time|GetWorldDeltaSeconds) (Variables|Default|GetInterpSpeed)))
  (Variables|Default|SetSeconds (+ (Variables|Default|GetSeconds) (Utilities|Time|GetWorldDeltaSeconds)))
  (if (Math|Float|InRange(Float) (.yaw (Transformation|GetActorRotation (Components|GetOwner))) (- _targetyaw 3.0) (+ _targetyaw 3.0))
    (Components|Tick|SetComponentTickEnabled false :!label _label)
    (elif (>= (Variables|Default|GetSeconds) 3.0) ; For safety
      (goto _label))))

(fn StartYawInterp
  (params (TargetYaw :type Float%20%28double-precision%29) (InterpSpeed :type Float%20%28single-precision%29))
  (Variables|Default|SetTargetYaw TargetYaw)
  (Variables|Default|SetInterpSpeed InterpSpeed)
  (Variables|Default|SetSeconds 0.0)
  (Components|Tick|SetComponentTickEnabled true)
  (return))