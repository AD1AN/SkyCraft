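; TEST_Tenbor is a test actor that turns into an essence pickup-style actor shortly after it begins play.
; On BeginPlay it enables physics simulation and collision on its mesh, then waits one second.
; It spawns a TEST_EssenceActor slightly above its current location, passing itself as Character along with its Island reference, then destroys itself after a DelayFrames node.
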(event EventBeginPlay
  (bind _mesh (Variables|Character|GetMesh))
  (Physics|SetSimulatePhysics _mesh true)
  (Collision|SetCollisionEnabled _mesh "QueryAndPhysics")
  (Utilities|FlowControl|Delay 1.0)
  (Game|SpawnActorfromClass "/Game/Blueprints/TEST_EssenceActor.TEST_EssenceActor_C" (Math|Transform|MakeTransform (+ (Transformation|GetActorLocation) "0.000000,0.000000,50.000000") "0, 0, 0" "1.000000,1.000000,1.000000") "Undefined" "MultiplyWithRoot" 0 self (Variables|Default|GetIsland) 0)
  (Class|LowEntryExtendedStandardLibrary|DelayFrames)
  (Actor|DestroyActor))

(fn ConstructionScript)