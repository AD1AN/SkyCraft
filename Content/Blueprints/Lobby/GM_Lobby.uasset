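; Lobby game mode that tracks joining players and lets a listen-server host move the session to another level.
; On PostLogin it stores each PC_Lobby in a player array and has that client create its widget.
; On a non-dedicated server, BeginPlay shows the W_LobbyHost widget with a mouse cursor.
; Its ServerTravel event builds a console command from the level name and the listen option.
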(event Custom|ServerTravel
  (params (LevelName :type String))
  (Development|ExecuteConsoleCommand (Utilities|String|Append "ServerTravel " (Utilities|String|Append LevelName "?listen")) 0))

(event EventBeginPlay
  (bind _returnvalue (Game|GetPlayerController 0))
  (if (not (Networking|IsDedicatedServer))
    (if (Networking|IsServer)
      (bind _returnvalue_2 (UserInterface|CreateWidget "/Game/Widgets/W_LobbyHost.W_LobbyHost_C" _returnvalue))
      (UserInterface|Viewport|AddtoViewport _returnvalue_2 0)
      (Variables|/Script/Engine.PlayerController|SetbShowMouseCursor _returnvalue true))))

(event EventPostLogin
  (params (NewPlayer :type Player%20Controller%20Object%20Reference))
  (bind _aspc_lobby (Utilities|Casting|CastToPC_Lobby NewPlayer))
  (bind _output_get (Variables|Default|SetLoginPlayerController _aspc_lobby))
  (Utilities|Array|Add (Variables|Default|GetPlayers) _output_get)
  (Default|ClientCreateWIdget (Variables|Default|GetLoginPlayerController)))

(fn ConstructionScript)