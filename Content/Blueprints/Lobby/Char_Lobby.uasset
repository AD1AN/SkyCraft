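; Char_Lobby is a lobby Blueprint, apparently the character, that exposes health and hunger queries.
; Getters return current Health and Hunger, and ratio functions divide each by its maximum without a zero check.
; ApplyDamage is a stub that ignores its input and returns false.
; GetMaxHealth returns a constant zero instead of the MaxHealth variable used by the health ratio, and the construction script is empty.
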(fn ConstructionScript)

(fn ApplyDamage
  (params (Damage :type Float%20%28double-precision%29))
  (return false))

(fn GetCurentHealth
  (return (Variables|Default|GetHealth)))

(fn GetHealthRatio
  (return (/ (Variables|Default|GetHealth) (Variables|Default|GetMaxHealth))))

(fn GetHunger
  (return (Variables|Default|GetHunger)))

(fn GetHungerRatio
  (return (/ (Variables|Default|GetHunger) (Variables|Default|GetMaxHunger))))

(fn GetMaxHealth
  (return 0.0))