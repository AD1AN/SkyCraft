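; Client-only actor that runs the loading screen while the player joins, muting master audio and destroying itself on dedicated servers.
; After login ends, it waits briefly, then tracks ungenerated Islands until each generates or is destroyed; non-shipping builds can skip this via a GameInstance flag.
; It then notifies the server once through BPPSS.
; The player-loaded callback hides the widget, enables input and fades audio in before the actor destroys itself.
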(event Custom|OnPlayerLoaded_Event
  (bind _bp_gis (Variables|Default|GetBP_GIS))
  (bind _bp_pcs (Variables|/Game/Blueprints/BP_GIS.BP_GIS_C|GetBP_PCS _bp_gis))
  (Default|HideLoadingScreen (Variables|Default|GetW_LoadingScreen) (delegate Custom|HideCompleted) 1.0)
  (Input|EnableInput (Variables|/Game/Blueprints/BP_PCS.BP_PCS_C|GetBP_PSS _bp_pcs) _bp_pcs)
  (Audio|SetSoundMixClassOverride "/Game/Audio/GameSoundMix.GameSoundMix" "/Game/Audio/Master.Master" (Variables|/Game/Blueprints/LocalSettings.LocalSettings_C|GetMasterVolume (Variables|/Game/Blueprints/BP_GIS.BP_GIS_C|GetLocalSettings (Variables|Default|GetBP_GIS))) 1.0 2.0 true)
  (Audio|PushSoundMixModifier "/Game/Audio/GameSoundMix.GameSoundMix"))

(event Custom|OnGenerated_Event
  (params (Island :type Island%20Object%20Reference))
  (Utilities|Array|RemoveItem (Variables|Default|GetLoadingIslands) Island)
  (CallFunction|IsLoad?))

(event Custom|OnDestroyed_Event
  (params (DestroyedActor :type Actor%20Object%20Reference))
  (bind _asisland (Utilities|Casting|CastToIsland DestroyedActor))
  (Utilities|Array|RemoveItem (Variables|Default|GetLoadingIslands) _asisland)
  (Utilities|Array|RemoveItem (Variables|Default|GetAllIslands) _asisland)
  (CallFunction|IsLoad?))

(event Custom|OnPlayerLoginEnded
  (if (Class|LowEntryExtendedStandardLibrary|ShippingBuild)
    (Default|SetLoadingStage (Variables|Default|GetW_LoadingScreen) 1 :!label _label)
    (Utilities|FlowControl|Delay 3.0) ; I am the greatest programmer!
    (bind _outactors (Actor|GetAllActorsOfClass "/Script/SkyCraft.Island"))
    (bind _output_get (Variables|Default|SetAllIslands _outactors))
    (bind _output_get_2 (Variables|Default|SetLoadingIslands _output_get))
    (bind (_arrayindex _arrayelement) (Utilities|Array|ReverseforEachLoop _output_get_2)
      (:LoopBody
        (if (Variables|/Script/SkyCraft.Island|GetbFullGenerated _arrayelement)
          (Utilities|Array|RemoveIndex (Variables|Default|GetLoadingIslands) _arrayindex)
          (else
            (EventDispatchers|AssignOnIslandFullGenerated _arrayelement (delegate Custom|OnGenerated_Event))
            (Game|AssignOnDestroyed _arrayelement (delegate Custom|OnDestroyed_Event)))))
      (:Completed
        (Default|SetLoadingStage (Variables|Default|GetW_LoadingScreen) 2)
        (CallFunction|IsLoad?)))
    (elif (Variables|/Game/Blueprints/BP_GIS.BP_GIS_C|GetEditorLoadingScreen (Variables|Default|GetBP_GIS))
      (goto _label)
      (else
        (CallFunction|HardLoad) ; Fast editor
      ))))

(event Custom|HideCompleted
  (Widget|RemovefromParent (Variables|Default|GetW_LoadingScreen))
  (Actor|DestroyActor))

(event Custom|IsLoad?
  (if (Utilities|Array|IsEmpty (Variables|Default|GetLoadingIslands))
    (Utilities|FlowControl|DoOnce false
      (:Completed
        (Default|SetLoadingStage (Variables|Default|GetW_LoadingScreen) 3)
        (EventDispatchers|AssignOnPlayerLoaded (Variables|/Game/Blueprints/BP_GIS.BP_GIS_C|GetBP_PSS (Variables|Default|GetBP_GIS)) (delegate Custom|OnPlayerLoaded_Event))
        (Default|ServerPlayerLoaded (Variables|/Game/Blueprints/BP_GIS.BP_GIS_C|GetBP_PSS (Variables|Default|GetBP_GIS)))))))

(event Custom|HardLoad
  (Utilities|FlowControl|DoOnce false
    (:Completed
      (Default|SetLoadingStage (Variables|Default|GetW_LoadingScreen) 3)
      (EventDispatchers|AssignOnPlayerLoaded (Variables|/Game/Blueprints/BP_GIS.BP_GIS_C|GetBP_PSS (Variables|Default|GetBP_GIS)) (delegate Custom|OnPlayerLoaded_Event))
      (Default|ServerPlayerLoaded (Variables|/Game/Blueprints/BP_GIS.BP_GIS_C|GetBP_PSS (Variables|Default|GetBP_GIS))))))

(event EventBeginActor
  (bind _asbp_gis (Utilities|Casting|CastToBP_GIS (Game|GetGameInstance)))
  (Variables|Default|SetBP_GIS _asbp_gis)
  (if (Networking|IsDedicatedServer)
    (Actor|DestroyActor)
    (else
      (Audio|SetSoundMixClassOverride "/Game/Audio/GameSoundMix.GameSoundMix" "/Game/Audio/Master.Master" 0.0 1.0 0.0 true)
      (Audio|PushSoundMixModifier "/Game/Audio/GameSoundMix.GameSoundMix")
      (bind _returnvalue (UserInterface|CreateWidget "/Game/Widgets/W_LoadingScreen.W_LoadingScreen_C" 0 self))
      (bind _output_get (Variables|Default|SetW_LoadingScreen _returnvalue))
      (UserInterface|Viewport|AddtoViewport _output_get 1000000)
      (EventDispatchers|BindEventtoOnPlayerLoginEnded (Variables|Default|GetBP_GIS) (delegate Custom|OnPlayerLoginEnded))
      (Default|SetLoadingStage (Variables|Default|GetW_LoadingScreen)))))

(fn ConstructionScript)