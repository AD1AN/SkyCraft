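; Suffocation is a component that damages the owning player's normal form when it falls far below the world.
; On the server, BeginPlay enables ticking and caches PFNormal from the owner's player form message.
; Each tick, while that form sits below a fixed Z threshold, it applies random damage tagged as Suffocation.
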(event EventBeginPlay
  (if (Networking|IsServer)
    (Components|Tick|SetComponentTickEnabled true)
    (bind _pf_normal (Class|BPIPlayerForm|GetPlayerForm(Message) (Components|GetOwner)))
    (Variables|Default|SetPF_Normal _pf_normal)))

(event EventTick
  (params (DeltaSeconds :type Float%20%28single-precision%29))
  (if (< (.z (Transformation|GetActorLocation (Variables|Default|GetPF_Normal))) -2e+04)
    (Class|HealthSystemInterface|ApplyDamage(Message) (Variables|Default|GetPF_Normal) (Utilities|Struct|MakeApplyDamageIn (Math|Random|RandomIntegerinRange 25 75) 0 "/Game/DataAssets/DamageCauser/Suffocation.Suffocation" 0 0))))