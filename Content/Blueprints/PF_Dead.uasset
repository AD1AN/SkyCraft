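; PF_Dead is the networked player form for a dead player, holding leftover Essence and Inventory that an interaction widget exposes.
; While possessed, it provides look-around, inventory UI and a life span countdown run by the server.
; Pressing E or expiry closes the eyes, then respawns the player on a new island form, pre-spawning chunks.
; Expiry destroys the body; otherwise it remains until unpossessed and empty, or timed out.
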(event Custom|Server_Respawn
  (params (Destroy :type Boolean))
  (Components|DestroyComponent (Variables|Default|GetNMBV_Update))
  (bind _spawned_pf_island (Default|SpawnPFIsland (Variables|Default|GetBP_PCS) true))
  (Default|SpawnChunks (Variables|/Game/Blueprints/PF_Island.PF_Island_C|GetGenerator_Islands _spawned_pf_island)) ; Force Spawn Chunks to avoid re-spawn
  (Default|MinusSpawnedChunks (Variables|Default|GetGenerator_Islands))
  (Default|SpawnChunks (Variables|/Game/Blueprints/PF_Island.PF_Island_C|GetGenerator_Essence _spawned_pf_island)) ; Force Spawn Chunks to avoid re-spawn
  (Default|MinusSpawnedChunks (Variables|Default|GetGenerator_Essence))
  (if Destroy
    (CallFunction|ServerSideDestroyPFDead)
    (else
      (Variables|/Game/Blueprints/BP_PAI.BP_PAI_C|SetPF_Dead (Variables|Default|GetBP_PAI) 0) ; empty
      (Variables|Default|SetBP_PCS 0) ; empty
      (if (and (== (Utilities|Array|Length (Variables|/Game/Blueprints/Inventory.Inventory_C|GetSlots (Variables|Default|GetInventory))) 0) (== (Class|AdianFL|EssenceTotal (Variables|Default|GetEssence)) 0))
        (CallFunction|ServerSideDestroyPFDead)))))

(event Custom|Client_Possessed
  (bind _returnvalue (UserInterface|CreateWidget "/Game/Widgets/W_PF_Dead.W_PF_Dead_C" (Variables|Default|GetBP_PCS) self))
  (bind _output_get (Variables|Default|SetW_PF_Dead _returnvalue))
  (UserInterface|Viewport|AddtoViewport _output_get 0)
  (Actor|Tick|SetActorTickEnabled true))

(event Custom|ServerSide_DestroyPF_Dead
  (CallFunction|MulticastLOCALWOutside)
  (Actor|DestroyActor))

(event Custom|REMOVE_Inventory_Event_0
  (params (RemovedIndex :type Integer))
  (Utilities|IsValid (Variables|Default|GetBP_PCS)
    (:Is%20Not%20Valid
      (if (and (<= (Class|AdianFL|EssenceTotal (Variables|Default|GetEssence)) 0) (== (Utilities|Array|Length (Variables|/Game/Blueprints/Inventory.Inventory_C|GetSlots (Variables|Default|GetInventory))) 0))
        (CallFunction|ServerSideDestroyPFDead)))))

(event Custom|Multicast_LOCAL_W_Outside
  (bind _local_cws_chardeadoutsideinventory (Variables|Default|GetLOCAL_CWS_CharDeadOutsideInventory))
  (Utilities|IsValid _local_cws_chardeadoutsideinventory
    (:Is%20Valid
      (Default|ClientSideDestroyWidget _local_cws_chardeadoutsideinventory))))

(event Custom|Multicast_Initialization
  (params (Essence :type Essence%20Structure) (InventorySlots :type Array%20of%20Inventory%20Slot%20Structures))
  (Variables|Default|SetEssence Essence)
  (Variables|/Game/Blueprints/Inventory.Inventory_C|SetSlots (Variables|Default|GetInventory) InventorySlots))

(event Custom|Multicast_SetCurrentLifeSpan%28Unreliable%29
  (params (CurrentLifeSpan :type Float%20%28double-precision%29))
  (Variables|Default|SetCurrentLifeSpan CurrentLifeSpan))

(event Custom|Client_SetLookRotation
  (params (LookRotation :type Rotator))
  (bind _output_get (Variables|Default|SetLookRotation LookRotation))
  (Transformation|SetWorldRotation (Variables|Default|GetSkySpringArm) _output_get false false))

(event Custom|Multicast_SetLookRotation%28Reliable%29
  (params (LookRotation :type Rotator))
  (bind _output_get (Variables|Default|SetLookRotation LookRotation))
  (Transformation|SetWorldRotation (Variables|Default|GetSkySpringArm) _output_get false false))

(event Custom|2CloseEyesCompleted
  (CallFunction|ServerRespawn true))

(event Custom|ShowBlackCompleted
  (CallFunction|ServerRespawn false))

(event Custom|EssenceChanged_Event_0
  (Utilities|IsValid (Variables|Default|GetBP_PCS)
    (:Is%20Not%20Valid
      (if (and (<= (Class|AdianFL|EssenceTotal (Variables|Default|GetEssence)) 0) (== (Utilities|Array|Length (Variables|/Game/Blueprints/Inventory.Inventory_C|GetSlots (Variables|Default|GetInventory))) 0))
        (CallFunction|ServerSideDestroyPFDead)))))

(event Custom|Client_EndLifeSpan
  (Default|CreateEyesTransition (Variables|Default|GetBP_PCS) (delegate Custom|2CloseEyesCompleted)))

(event Custom|Server_EndLifeSpan
  (Utilities|IsValid (Variables|Default|GetBP_PCS)
    (:Is%20Valid
      (CallFunction|ClientEndLifeSpan))
    (:Is%20Not%20Valid
      (CallFunction|ServerSideDestroyPFDead))))

(event Custom|Mutlicast_InitSetup
  (params (Essence :type Essence%20Structure) (InventorySlots :type Array%20of%20Inventory%20Slot%20Structures))
  (Variables|Default|SetEssence Essence)
  (Variables|/Game/Blueprints/Inventory.Inventory_C|SetSlots (Variables|Default|GetInventory) InventorySlots))

(event EventPossessed
  (params (NewController :type Controller%20Object%20Reference))
  (Default|MulticastPlayerFormPossessed (Variables|Default|GetBP_PAI) "Dead" self)
  (CallFunction|ClientPossessed)
  (Game|Player|SetViewTargetwithBlend (Variables|Default|GetBP_PCS) self 0.0 "VTBlend_Linear" 0.0 false)
  (Actor|Tick|SetActorTickEnabled true))

(event EventBeginPlay
  (if (Networking|IsServer)
    (EventDispatchers|AssignEssenceChanged (delegate Custom|EssenceChanged_Event_0))
    (EventDispatchers|AssignREMOVEInventory (Variables|Default|GetInventory) (delegate Custom|REMOVE_Inventory_Event_0))))

(event EventTick
  (params (DeltaSeconds :type Float%20%28single-precision%29))
  (bind _w_pf_dead (Variables|Default|GetW_PF_Dead))
  (Utilities|IsOwner
    (:Server
      (if (<= (Variables|Default|GetCurrentLifeSpan) 0.0)
        (Utilities|FlowControl|DoOnce false
          (:Completed
            (CallFunction|ServerEndLifeSpan)))
        (else
          (bind _output_get (Variables|Default|SetCurrentLifeSpan (- (Variables|Default|GetCurrentLifeSpan) (Utilities|Time|GetWorldDeltaSeconds))))
          (CallFunction|MulticastSetCurrentLifeSpan(Unreliable) _output_get))))
    (:OwningClient
      (Transformation|SetWorldRotation (Variables|Default|GetSkySpringArm) (Variables|Default|GetLookRotation) false false)
      (Default|SetProgress (Variables|/Game/Widgets/W_PF_Dead.W_PF_Dead_C|GetDissolveProgress _w_pf_dead) (/ (Variables|Default|GetCurrentLifeSpan) (Variables|Default|GetMaxLifeSpan)))
      (Rendering|Components|TextRender|SetText (Variables|/Game/Widgets/W_PF_Dead.W_PF_Dead_C|GetRemainLifeSpan _w_pf_dead) (Utilities|Text|FormatText "{0}:{1}" (Utilities|Text|ToText(Integer) (Math|Timespan|GetMinutes (Math|Timespan|MakeTimespan 0 0 0 (Math|Float|Truncate (Variables|Default|GetCurrentLifeSpan)) 0)) false true 2 2) (Utilities|Text|ToText(Integer) (Math|Timespan|GetSeconds (Math|Timespan|MakeTimespan 0 0 0 (Math|Float|Truncate (Variables|Default|GetCurrentLifeSpan)) 0)) false true 2 2))))))

(event EventClientUnpossess
  (bind _w_pf_dead (Variables|Default|GetW_PF_Dead))
  (Utilities|IsValid _w_pf_dead
    (:Is%20Valid
      (Widget|RemovefromParent _w_pf_dead))
    (:Is%20Not%20Valid
      _))
  (Utilities|IsValid (Variables|Default|GetW_CharDeadInsideInventory)
    (:Is%20Valid
      (Widget|RemovefromParent (Variables|Default|GetW_CharDeadInsideInventory))
      (Variables|Default|SetW_CharDeadInsideInventory 0) ; empty
    )
    (:Is%20Not%20Valid
      _))
  (Utilities|Platform|CollectGarbage)
  (Actor|Tick|SetActorTickEnabled false))

(event EventClientAfterPossess
  (Default|CallAfterPFPossessed (Variables|Default|GetBP_PCS)))

(event Input|ActionEvents|InputActionInventory
  (params (Key :type Key%20Structure))
  (bind _bp_pcs (Variables|Default|GetBP_PCS))
  (:Pressed
    (Utilities|IsValid (Variables|Default|GetW_CharDeadInsideInventory)
      (:Is%20Valid
        (Widget|RemovefromParent (Variables|Default|GetW_CharDeadInsideInventory))
        (Variables|Default|SetW_CharDeadInsideInventory 0) ; empty
        (Utilities|Platform|CollectGarbage))
      (:Is%20Not%20Valid
        (bind _returnvalue (UserInterface|CreateWidget "/Game/Widgets/W_PF_DeadInsideInventory.W_PF_DeadInsideInventory_C" _bp_pcs _bp_pcs self))
        (bind _output_get (Variables|Default|SetW_CharDeadInsideInventory _returnvalue))
        (UserInterface|Viewport|AddtoViewport _output_get 0)))))

(event Input|AxisEvents|InputAxisLookUp
  (params (AxisValue :type Float%20%28single-precision%29))
  (Variables|Default|SetLookRotation (Math|Rotator|MakeRotator (.roll (Variables|Default|GetLookRotation)) (Math|Float|ClampAngle (+ (* AxisValue -2.5) (.pitch (Variables|Default|GetLookRotation))) -9e+01 9e+01) (.yaw (Variables|Default|GetLookRotation)))))

(event Input|AxisEvents|InputAxisTurn
  (params (AxisValue :type Float%20%28single-precision%29))
  (Variables|Default|SetLookRotation (Math|Rotator|MakeRotator (.roll (Variables|Default|GetLookRotation)) (.pitch (Variables|Default|GetLookRotation)) (+ (* AxisValue 2.5) (.yaw (Variables|Default|GetLookRotation))))))

(event Input|KeyboardEvents|E
  (params (Key :type Key%20Structure))
  (:Pressed
    (Default|CreateEyesTransition (Variables|Default|GetBP_PCS) (delegate Custom|ShowBlackCompleted) self)
    (Input|DisableInput (Variables|Default|GetBP_PCS))))

(fn ConstructionScript)

(fn OnRepEssence
  (Default|CallEssenceChanged))

(fn GetIDAttachedtoIA
  (bind _attachedtoia (Variables|Default|GetAttachedToIA))
  (Utilities|IsValid _attachedtoia
    (:Is%20Valid
      (return (Variables|/Game/Blueprints/IslandArchon.IslandArchon_C|GetID_IA _attachedtoia)))
    (:Is%20Not%20Valid
      (return -1))))

(fn GetLocationbyIA
  (Utilities|IsValid (Variables|Default|GetAttachedToIA)
    (:Is%20Valid
      (return (Math|Transform|InverseTransformLocation (Transformation|GetActorTransform (Variables|Default|GetAttachedToIA)) (Transformation|GetActorLocation))) ; Relative
    )
    (:Is%20Not%20Valid
      (return (Transformation|GetActorLocation)) ; World
    )))

(fn CameraComponents
  (return (Variables|Default|GetSkySpringArm) (Variables|Default|GetCamera)))

(fn ClientInteractBP
  (params (InteractKey :type EInteractKey%20Enum :default "Interact1") (Pawn :type Pawn%20Object%20Reference) (BP_PAI :type BP%20PAI%20Object%20Reference))
  (bind _returnvalue (UserInterface|CreateWidget "/Game/Widgets/CWS/CWS_PF_DeadOutsideInventory.CWS_PF_DeadOutsideInventory_C" 0 self Pawn))
  (bind _output_get (Variables|Default|SetLOCAL_CWS_CharDeadOutsideInventory _returnvalue))
  (UserInterface|Viewport|AddtoViewport _output_get 0)
  (Default|AddCWS BP_PAI _output_get true true "NewEnumerator2")
  (Default|SetMousetoCenter BP_PAI)
  (return false))

(fn ClientInterruptBP
  (params (InterruptedBy :type EInterruptedBy%20Enum :default "Player") (InteractKey :type EInteractKey%20Enum :default "Interact1") (Pawn :type Pawn%20Object%20Reference) (BP_PAI :type BP%20PAI%20Object%20Reference))
  (Default|RemoveCWS BP_PAI (Variables|Default|GetLOCAL_CWS_CharDeadOutsideInventory) true true)
  (Variables|Default|SetLOCAL_CWS_CharDeadOutsideInventory 0) ; empty
  (return true))

(fn ConsumeEssence
  (params (Essence :type Essence%20Structure))
  (return false))

(fn GetBPPAI
  (return (Variables|Default|GetBP_PAI)))

(fn GetBPPCS
  (return (Variables|Default|GetBP_PCS)))

(fn GetInventory
  (return (Variables|Default|GetInventory)))

(fn GetPlayerForm
  (return 0 0 0 self))

(fn GetEssence
  (return (Variables|Default|GetEssence)))

(fn GetInteractLocation
  (return (Transformation|GetActorLocation)))

(fn GetInteractSystem
  (return (Variables|Default|GetInteractSystem)))

(fn GetLookRotation
  (return (Variables|Default|GetLookRotation)))

(fn ServerInteractBP
  (params (InteractKey :type EInteractKey%20Enum :default "Interact1") (Pawn :type Pawn%20Object%20Reference) (BP_PAI :type BP%20PAI%20Object%20Reference))
  (return false))

(fn ServerInterruptBP
  (params (InterruptedBy :type EInterruptedBy%20Enum :default "Player") (InteractKey :type EInteractKey%20Enum :default "Interact1") (Pawn :type Pawn%20Object%20Reference) (BP_PAI :type BP%20PAI%20Object%20Reference))
  (return false))

(fn SetEssence(Server)
  (params (Essence :type Essence%20Structure))
  (bind _output_get (Variables|Default|SetEssence Essence))
  (return _output_get))

(fn SetLookRotation
  (params (LookRotation :type Rotator :default "0, 0, 0"))
  (bind _output_get (Variables|Default|SetLookRotation LookRotation))
  (return _output_get))