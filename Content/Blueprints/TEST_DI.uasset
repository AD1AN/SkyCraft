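; TEST_DI is a test Blueprint for a physics sphere that stops when it lands on an upward-facing surface.
; On BeginPlay it attaches a component, keeping world transform, to the Attach reference's SceneComponent tagged "AttachedPhysicsObjects".
; On Hit it measures the angle between the hit normal and world up, putting the Sphere's rigid body to sleep unless the surface is near-vertical or downward-facing.
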(event Collision|EventHit
  (params (MyComp :type Primitive%20Component%20Object%20Reference) (Other :type Actor%20Object%20Reference) (OtherComp :type Primitive%20Component%20Object%20Reference) (bSelfMoved :type Boolean) (HitLocation :type Vector :default "0, 0, 0") (HitNormal :type Vector :default "0, 0, 0") (NormalImpulse :type Vector :default "0, 0, 0") (Hit :type Hit%20Result%20Structure%20%28by%20ref%29))
  (if (<= (Class|KismetMathLibrary|DegAcos (Math|Vector|DotProduct HitNormal (Math|Vector|VectorUp))) 89.0)
    (Class|PrimitiveComponent|PutRigidBodytoSleep (Variables|Default|GetSphere) "None")))

(event EventBeginPlay
  (Transformation|AttachComponentToComponent (Class|Actor|FindComponentbyTag (Variables|Default|GetAttach) "/Script/Engine.SceneComponent" "AttachedPhysicsObjects") "None" "KeepWorld" "KeepWorld" "KeepWorld" true))

(fn ConstructionScript)