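; BP_Ruce is a passive NPC that roams randomly and flees when a player damages it.
; Tick, enabled on the server in BeginPlay, switches between roaming with pauses and fleeing, using DoOnce gates around AIMoveTo.
; Flight targets a reachable point opposite the attacker, falling back to a random nearby one, until a timer expires or the attacker becomes invalid.
; ApplyDamage restarts flight on player hits, subtracts health and destroys the actor at zero.
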(event EventBeginPlay
  (if (Networking|IsServer)
    (Actor|Tick|SetActorTickEnabled true)))

(event EventTick
  (params (DeltaSeconds :type Float%20%28single-precision%29))
  (bind _returnvalue (Transformation|GetActorLocation))
  (bind _returnvalue_2 (Transformation|GetActorLocation))
  (bind _runawayfrom (Variables|Default|GetRunAwayFrom))
  (bind _returnvalue_3 (Transformation|GetActorLocation _runawayfrom))
  (bind _returnvalue_4 (Math|Rotator|FindLookatRotation _returnvalue _returnvalue_3))
  (bind _returnvalue_5 (- (.yaw _returnvalue_4) 1.8e+02))
  (bind _returnvalue_6 (Math|Rotator|MakeRotator 0.0 0.0 _returnvalue_5))
  (bind _returnvalue_7 (Math|Vector|GetForwardVector _returnvalue_6))
  (bind _returnvalue_8 (* _returnvalue_7 1e+03))
  (bind _returnvalue_9 (+ _returnvalue_8 _returnvalue_2))
  (bind (_randomlocation _returnvalue_10) (AI|Navigation|GetRandomReachablePointinRadius _returnvalue_9 5e+02 0 0))
  (if (Variables|Default|GetRunAway)
    (bind _output_get (Variables|Default|SetRunAwayTime (+ (Variables|Default|GetRunAwayTime) (Utilities|Time|GetWorldDeltaSeconds))))
    (if (>= _output_get 3e+01)
      _
      (else
        (Utilities|IsValid (Variables|Default|GetRunAwayFrom)
          (:Is%20Valid
            (Utilities|FlowControl|DoOnce false :!label _label
              (:Completed
                (AI|AIMoveTo self (Math|Vector|SelectVector _randomlocation (.RandomLocation (AI|Navigation|GetRandomReachablePointinRadius _returnvalue_2 5e+02 0 0)) _returnvalue_10) 0 5.0 false
                  (:OnSuccess
                    (goto _label Reset))
                  (:OnFail
                    (goto _label Reset))))))
          (:Is%20Not%20Valid
            _))))
    (Variables|Default|SetRunAway false)
    (Variables|Default|SetRunAwayTime 0.0)
    (else
      ;[1 1 1] Roaming
      (Utilities|FlowControl|DoOnce false :!label _label_2
        (:Completed
          (AI|AIMoveTo self (.RandomLocation (AI|Navigation|GetRandomReachablePointinRadius (Transformation|GetActorLocation) 5e+02 0 0)) 0 5.0 false
            (:OnSuccess
              _)
            (:OnFail
              _))
          (Utilities|FlowControl|Delay 2.0)
          (goto _label_2 Reset))))))

(fn ConstructionScript)

(fn ApplyDamage
  (params (BaseDamage :type Integer) (DamageCauserInfo :type DA%20Damage%20Causer%20Info%20Object%20Reference) (DamageCauser :type Object%20Object%20Reference) (WhoCauser :type Actor%20Object%20Reference) (Damage :type Integer))
  (Utilities|FlowControl|Sequence
    (:then_0
      (switch Utilities|FlowControl|Switch|SwitchonE_DamageDealerType (LocalVariables|GetDealerType)
        (:NewEnumerator0
          (Variables|Default|SetRunAwayFrom (LocalVariables|GetActorDealer))
          (Variables|Default|SetRunAway true)
          (Variables|Default|SetRunAwayTime 0.0))))
    (:then_1
      (bind _output_get (Variables|Default|SetCurrentHealth (- (Variables|Default|GetCurrentHealth) Damage)))
      (if (<= _output_get 0.0)
        (Actor|DestroyActor)
        (return true (<= _output_get 0.0))))))

(fn GetDamageModifiers
  (return 0))