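; Inventory component that stores item stacks in a slot array, with functions to add, remove, consume, count and swap items.
; Adding reads stacking rules from the item's DataTable, tops up matching stacks, then takes an empty slot (row name "None").
; Slot writes go through multicast events that update each machine's array and fire change notifications.
; Swap routes both writes through the player controller's server call, allowing exchanges between two inventory components.
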(event Custom|Multicast_REMOVE_Inventory
  (params (RemoveIndex :type Integer))
  (Utilities|Array|RemoveIndex (Variables|Default|GetInventory) RemoveIndex)
  (Default|CallREMOVEInventory RemoveIndex))

(event Custom|Multicast_SAE_Inventory
  (params (Index :type Integer) (Item :type S%20Inventory%20Slot%20Structure))
  (Utilities|Array|SetArrayElem (Variables|Default|GetInventory) Index Item)
  (Default|CallSAEInventory Index))

(event Custom|Multicast_ADD_Inventory
  (params (Item :type S%20Inventory%20Slot%20Structure%20%28by%20ref%29))
  (bind _returnvalue (Utilities|Array|Add (Variables|Default|GetInventory) Item))
  (Default|CallADDInventory _returnvalue))

(event Custom|Server_AddToInventory
  (params (Item :type S%20Inventory%20Slot%20Structure))
  (CallFunction|AddtoInventory Item))

(event EventTick
  (params (DeltaSeconds :type Float%20%28single-precision%29)))

(fn AddtoInventory
  (params (Item :type S%20Inventory%20Slot%20Structure))
  (bind _output_get (LocalVariables|Set_Item Item))
  (LocalVariables|Set_LeftQuantity (.Quantity (CallFunction|BreakSInventorySlot _output_get)))
  (bind _output_get_2 (LocalVariables|Set_ItemRowName (.Item%20Row%20Name (CallFunction|BreakSInventorySlot _output_get))))
  (bind _returnvalue (Utilities|GetDataTableRow (.Item%20Data%20Table (CallFunction|BreakSInventorySlot _output_get)) _output_get_2)
    (:then
      (if (.Stacking (Utilities|Struct|BreakS_Item _returnvalue)) ; If stacking
        (for (_array_element _array_index) (Variables|Default|GetInventory) ; Search for similar
          (if (and (Utilities|Name|Equal(Name) (.rowname (.Item (Utilities|Struct|BreakS_InventorySlot _array_element))) (LocalVariables|Get_ItemRowName)) (< (.Quantity (Utilities|Struct|BreakS_InventorySlot _array_element)) (.MaxStacking (Utilities|Struct|BreakS_Item _returnvalue))))
            (if (> (+ (.Quantity (Utilities|Struct|BreakS_InventorySlot _array_element)) (LocalVariables|Get_LeftQuantity)) (.MaxStacking (Utilities|Struct|BreakS_Item _returnvalue))) ; If stack overflow
              (LocalVariables|Set_LeftQuantity (- (+ (.Quantity (Utilities|Struct|BreakS_InventorySlot _array_element)) (LocalVariables|Get_LeftQuantity)) (.MaxStacking (Utilities|Struct|BreakS_Item _returnvalue))))
              (CallFunction|MulticastSAEInventory _array_index (Utilities|Struct|MakeS_InventorySlot (.Item (Utilities|Struct|BreakS_InventorySlot _array_element)) (.MaxStacking (Utilities|Struct|BreakS_Item _returnvalue)) 1e+05))
              (else
                (CallFunction|MulticastSAEInventory _array_index (Utilities|Struct|MakeS_InventorySlot (.Item (Utilities|Struct|BreakS_InventorySlot _array_element)) (+ (.Quantity (Utilities|Struct|BreakS_InventorySlot _array_element)) (LocalVariables|Get_LeftQuantity)) 1e+05))
                (return true 0)))))
        (for (_array_element_2 _array_index_2) (Variables|Default|GetInventory) ; Search for empty
          (if (Utilities|Name|Equal(Name) (.rowname (.Item (Utilities|Struct|BreakS_InventorySlot _array_element_2))) "None")
            (CallFunction|MulticastSAEInventory _array_index_2 (Utilities|Struct|MakeS_InventorySlot (.item (LocalVariables|Get_Item)) (LocalVariables|Get_LeftQuantity) 1e+05))
            (return true 0)))
        (return false (LocalVariables|Get_LeftQuantity))
        (else
          (bind (_array_element_3 _array_index_3) (Utilities|Array|ForEachLoopwithBreak (Variables|Default|GetInventory)) ; Search for empty
            (:LoopBody
              (if (Utilities|Name|Equal(Name) (.rowname (.Item (Utilities|Struct|BreakS_InventorySlot _array_element_3))) "None")
                (CallFunction|MulticastSAEInventory _array_index_3 (LocalVariables|Get_Item))
                (return true 0)))))))))

(fn RemovefromInventory
  (params (RemoveIndex :type Integer) (RemoveQuantity :type Integer))
  (bind (_array_element _array_index) (Utilities|Array|ForEachLoopwithBreak (Variables|Default|GetInventory) :!label _label)
    (:LoopBody
      (if (== _array_index RemoveIndex)
        (if (> (- (.Quantity (CallFunction|BreakSInventorySlot _array_element)) RemoveQuantity) 0)
          (CallFunction|MulticastSAEInventory RemoveIndex (Utilities|Struct|MakeS_InventorySlot (Utilities|Struct|MakeDataTableRowHandle (.Item%20Data%20Table (CallFunction|BreakSInventorySlot _array_element)) (.Item%20Row%20Name (CallFunction|BreakSInventorySlot _array_element))) (- (.Quantity (CallFunction|BreakSInventorySlot _array_element)) RemoveQuantity) (.Durability (CallFunction|BreakSInventorySlot _array_element))))
          (goto _label Break)
          (else
            (CallFunction|MulticastSAEInventory RemoveIndex (Utilities|Struct|MakeS_InventorySlot "(DataTable=DataTable'\"/Game/Inventory/DT_Items.DT_Items\"',RowName=\"\")" (- (.Quantity (CallFunction|BreakSInventorySlot _array_element)) RemoveQuantity) 1e+05))
            (goto _label Break)))))))

(fn WastefromInventory
  (params (Item :type S%20Inventory%20Slot%20Structure))
  (LocalVariables|SetHowManyNeed (.Quantity (Utilities|Struct|BreakS_InventorySlot Item)))
  (bind (_array_element _array_index) (Utilities|Array|ForEachLoopwithBreak (Variables|Default|GetInventory) :!label _label)
    (:LoopBody
      (if (== (.rowname (.Item (Utilities|Struct|BreakS_InventorySlot _array_element))) (.Item%20Row%20Name (CallFunction|BreakSInventorySlot Item)))
        (bind _output_get (LocalVariables|SetHowManyNeed (- (LocalVariables|GetHowManyNeed) (.Quantity (Utilities|Struct|BreakS_InventorySlot _array_element)))))
        (if (== _output_get 0)
          (CallFunction|MulticastSAEInventory _array_index)
          (goto _label Break)
          (elif (< _output_get 0)
            (CallFunction|MulticastSAEInventory _array_index (Utilities|Struct|MakeS_InventorySlot (.item (Utilities|Array|Get(acopy) (Variables|Default|GetInventory) _array_index)) (Math|Integer|Absolute(Integer) (LocalVariables|GetHowManyNeed)) 1e+05))
            (goto _label Break)))))))

(fn HMH
  (params (ItemRowName :type Name))
  (bind _array_element (Utilities|Array|ForEachLoopwithBreak (Variables|Default|GetInventory))
    (:LoopBody
      (if (== (.rowname (.Item (Utilities|Struct|BreakS_InventorySlot _array_element))) ItemRowName)
        (LocalVariables|Set_HMH (+ (.Quantity (Utilities|Struct|BreakS_InventorySlot _array_element)) (LocalVariables|Get_HMH)))))
    (:Completed
      (return (LocalVariables|Get_HMH)))))

(fn Swap
  (params (InventoryIndex :type Integer) (DraggedInventoryIndex :type Integer) (DraggedInventoryComponent :type AC%20Inventory%20Object%20Reference%20%28by%20ref%29) (PC_Sky :type PC%20Sky%20Object%20Reference%20%28by%20ref%29))
  (LocalVariables|SetItem (Utilities|Array|Get(acopy) (Variables|Default|GetInventory) InventoryIndex))
  (bind _output_get (LocalVariables|SetDraggedItem (Utilities|Array|Get(acopy) (Variables|AC_Inventory_C|GetInventory DraggedInventoryComponent) DraggedInventoryIndex)))
  (Default|ServerMulticastSAEInventory PC_Sky self InventoryIndex _output_get)
  (Default|ServerMulticastSAEInventory PC_Sky DraggedInventoryComponent DraggedInventoryIndex (LocalVariables|GetItem))
  (return))

(fn CheckEmptySlots
  (for (_array_element _array_index) (Variables|Default|GetInventory)
    (if (Utilities|Name|Equal(Name) (.Item%20Row%20Name (CallFunction|BreakSInventorySlot _array_element)) "None")
      (Utilities|Array|Add (LocalVariables|Get_EmptySlots) _array_index)))
  (return (LocalVariables|Get_EmptySlots)))

(fn RemoveIndex
  (params (Index :type Integer))
  (Utilities|Array|RemoveIndex (Variables|Default|GetInventory) Index))