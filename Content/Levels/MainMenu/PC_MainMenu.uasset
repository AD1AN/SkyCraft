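; Main menu player controller that manages a stack of open widgets for back navigation with Escape.
; BeginPlay adds the default Enhanced Input mapping context, and other code can push or remove widgets through the stack functions.
; Escape removes the top widget from both stack and parent.
; After each removal, any new top widget receives AssignInputActionsMessage, and a failed stack removal prints a debug message.
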(event EventBeginPlay
  (Input|AddMappingContext (PlayerController|LocalPlayerSubsystems|GetEnhancedInputLocalPlayerSubsystem) "/Game/Misc/EnhancedInput/DefaultMappingContext.DefaultMappingContext" 0 (Utilities|Struct|MakeModifyContextOptions true true true)))

(event Input|KeyboardEvents|Escape
  (params (Key :type Key%20Structure :default "None"))
  (bind _stackwidgets (Variables|Default|GetStackWidgets))
  (:Pressed
    (if (not (Utilities|Array|IsEmpty (Variables|Default|GetStackWidgets))) ; If empty
      (CallFunction|RemoveStackWidget (Utilities|Array|Get(acopy) _stackwidgets (Utilities|Array|LastIndex _stackwidgets)) true true))))

(fn ConstructionScript)

(fn AddStackWidget
  (params (AddStackWidget :type User%20Widget%20Object%20Reference))
  (Utilities|Array|Add (Variables|Default|GetStackWidgets) AddStackWidget))

(fn RemoveStackWidget
  (params (RemoveStackWidget :type User%20Widget%20Object%20Reference) (RemoveFromStack :type Boolean) (RemoveFromParent :type Boolean))
  (bind _stackwidgets (Variables|Default|GetStackWidgets))
  (bind _returnvalue (Utilities|Array|LastIndex _stackwidgets))
  (Utilities|FlowControl|Sequence
    (:then_0
      (if RemoveFromStack
        (bind _returnvalue_2 (Utilities|Array|RemoveItem (Variables|Default|GetStackWidgets) RemoveStackWidget))
        (if (not _returnvalue_2)
          (Development|PrintString (Utilities|String|Append "Can't find in CWS: " (Utilities|GetDisplayName RemoveStackWidget)) true true "(R=1.000000,G=0.000000,B=0.008937,A=1.000000)" 25.0))))
    (:then_1
      (if RemoveFromParent
        (Widget|RemovefromParent RemoveStackWidget)))
    (:then_2
      (if (not (== _returnvalue -1)) ; If empty
        (Class|BPIInputAction|AssignInputActions(Message) (Utilities|Array|Get(acopy) (Variables|Default|GetStackWidgets) _returnvalue))))))