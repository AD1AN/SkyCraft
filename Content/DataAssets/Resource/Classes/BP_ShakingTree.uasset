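; Tree resource actor that shakes when its entity component takes damage.
; The first hit caches the actor's initial rotation, and every hit plays the Shaking timeline from the start.
; The timeline lerps rotation from that cached value toward a slight roll at the same yaw, then restores the original on finish.
; Caching only once keeps repeated hits from drifting the tree's resting rotation.
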(event OnDamage(EntityComponent)
  (params (DamageInfo :type Damage%20Info%20Structure))
  (if (Variables|Default|GethaveRotation)
    (bind _newtrack_0 (Timeline|Shaking PlayFromStart)
      (:Update
        (Transformation|SetActorRotation (Math|Rotator|Lerp(Rotator) (Variables|Default|GetInitialRotation) (Math|Rotator|MakeRotator 1.0 0.0 (.yaw (Variables|Default|GetInitialRotation))) _newtrack_0) true))
      (:Finished
        (Transformation|SetActorRotation (Variables|Default|GetInitialRotation) true)))
    (else
      (Variables|Default|SetInitialRotation (Transformation|GetActorRotation))
      (Variables|Default|SethaveRotation true)
      (Timeline|Shaking PlayFromStart))))

(fn ConstructionScript)