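; BP_SingleStone is an interactable stone that a pawn picks up by hand into its inventory.
; Server interaction inserts one I_Stone into the pawn's tagged InventoryComponent, then multicasts pickup sound and Niagara FX through the GameState, attached to the stone's parent actor, and destroys the stone.
; If insertion fails, the stone's EntityComponent dies with a StoneAxe damage action instead.
; Client interaction and both interrupt handlers just return false.
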(fn ConstructionScript)

(fn ClientInteractBP
  (params (InteractKey :type EInteractKey%20Enum :default "Interact1") (Pawn :type Pawn%20Object%20Reference) (BP_PSS :type BP%20PSS%20Object%20Reference))
  (return false))

(fn ClientInterruptBP
  (params (InterruptedBy :type EInterruptedBy%20Enum :default "Player") (InteractKey :type EInteractKey%20Enum :default "Interact1") (Pawn :type Pawn%20Object%20Reference) (BP_PSS :type BP%20PSS%20Object%20Reference))
  (return false))

(fn ServerInteractBP
  (params (InteractKey :type EInteractKey%20Enum :default "Interact1") (Pawn :type Pawn%20Object%20Reference) (BP_PSS :type BP%20PSS%20Object%20Reference))
  (bind _returnvalue (Class|Actor|FindComponentbyTag Pawn "/Script/SkyCraft.InventoryComponent" "Inventory"))
  (bind _returnvalue_2 (Actor|GetAttachParentActor))
  (Utilities|IsValid _returnvalue
    (:Is%20Valid
      (bind _returnvalue_3 (Class|InventoryComponent|InsertSlot _returnvalue (Utilities|Struct|MakeSlot "/Game/DataAssets/Item/I_Stone.I_Stone" 1 0)))
      (if _returnvalue_3
        (bind _asgss (Utilities|Casting|CastToGSS (Game|GetGameState))
          (:then
            _)
          (:CastFailed
            _))
        (Class|GSS|MulticastSpawnFXAttached _asgss (Utilities|Struct|MakeCue "/Game/Audio/SFX/HandstonePickup.HandstonePickup" "/Game/Niagara/NS_HandStonePickup.NS_HandStonePickup" false 0) (Class|AdianFL|ToLocalSpace (Transformation|GetActorLocation) _returnvalue_2) _returnvalue_2 "/Game/Audio/NormalAttenuation.NormalAttenuation")
        (Actor|DestroyActor)
        (return true)
        (else
          (Class|EntityComponent|AuthDie (Variables|Default|GetEntityComponent) (Utilities|Struct|MakeDamageInfo "/Game/DataAssets/DamageAction/StoneAxe.StoneAxe" 0 "0.000000,0.000000,0.000000" 0.0)))))
    (:Is%20Not%20Valid
      (Development|PrintString "Inventory not found" true true "(R=1.000000,G=0.000000,B=0.008937,A=1.000000)" 25.0))))

(fn ServerInterruptBP
  (params (InterruptedBy :type EInterruptedBy%20Enum :default "Player") (InteractKey :type EInteractKey%20Enum :default "Interact1") (Pawn :type Pawn%20Object%20Reference) (BP_PSS :type BP%20PSS%20Object%20Reference))
  (return false))