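; BP_Drevinika is a harvestable resource that gives the interacting pawn a random stack of Drevinika items.
; The server inserts the items into the pawn's tagged Inventory component, then clears Fruits and multicasts a picking sound through the game state.
; A multicast timeline briefly tilts the actor from its cached rotation and restores it.
; Fruits' RepNotify toggles mesh visibility and, on authority, interactability.
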(event Custom|Multicast_PickingFX
  (if (Variables|Default|GethaveRotation)
    (bind _newtrack_0 (Timeline|Timeline PlayFromStart)
      (:Update
        (Transformation|SetActorRotation (Math|Rotator|Lerp(Rotator) (Variables|Default|GetInitialRotation) (Math|Rotator|MakeRotator 1.0 0.0 (.yaw (Variables|Default|GetInitialRotation))) _newtrack_0) true))
      (:Finished
        (Transformation|SetActorRotation (Variables|Default|GetInitialRotation) true)))
    (else
      (Variables|Default|SetInitialRotation (Transformation|GetActorRotation))
      (Variables|Default|SethaveRotation true)
      (Timeline|Timeline PlayFromStart))))

(fn ConstructionScript)

(fn OnRepFruits
  (Rendering|SetVisibility (Variables|Default|GetStaticMesh) (Variables|Default|GetFruits) false)
  (Networking|SwitchHasAuthority
    (:Authority
      (Class|InteractComponent|SetInteractable (Variables|Default|GetInteractComponent) (Variables|Default|GetFruits)))))

(fn ClientInteractBP
  (params (InteractKey :type EInteractKey%20Enum :default "Interact1") (Pawn :type Pawn%20Object%20Reference) (BP_PSS :type BP%20PSS%20Object%20Reference))
  (return false))

(fn ClientInterruptBP
  (params (InterruptedBy :type EInterruptedBy%20Enum :default "Player") (InteractKey :type EInteractKey%20Enum :default "Interact1") (Pawn :type Pawn%20Object%20Reference) (BP_PSS :type BP%20PSS%20Object%20Reference))
  (return false))

(fn ServerInteractBP
  (params (InteractKey :type EInteractKey%20Enum :default "Interact1") (Pawn :type Pawn%20Object%20Reference) (BP_PSS :type BP%20PSS%20Object%20Reference))
  (bind _returnvalue (Class|Actor|FindComponentbyTag Pawn "/Script/SkyCraft.Inventory" "Inventory"))
  (bind _returnvalue_2 (Actor|GetAttachParentActor))
  (if (Variables|Default|GetFruits)
    (Utilities|IsValid _returnvalue
      (:Is%20Valid
        (bind _returnvalue_3 (Class|Inventory|InsertSlot _returnvalue (Utilities|Struct|MakeSlot "/Game/DataAssets/Item/I_Drevinika.I_Drevinika" (Math|Conversions|ToByte(Integer) (Math|Random|RandomIntegerinRange 5 10)) 0)))
        (if _returnvalue_3
          (CallFunction|MulticastPickingFX)
          (bind _asgss (Utilities|Casting|CastToGSS (Game|GetGameState)))
          (Class|GSS|MulticastSpawnFXAttached _asgss (Utilities|Struct|MakeFX "/Game/Audio/SFX/Mattock_AddFoliage.Mattock_AddFoliage" 0 false 0) (Class|AdianFL|ToLocalSpace (Transformation|GetActorLocation) _returnvalue_2) _returnvalue_2 "/Game/Audio/NormalAttenuation.NormalAttenuation")
          (Variables|Default|SetFruits false)
          (Networking|ForceNetUpdate)
          (return true))))))

(fn ServerInterruptBP
  (params (InterruptedBy :type EInterruptedBy%20Enum :default "Player") (InteractKey :type EInteractKey%20Enum :default "Interact1") (Pawn :type Pawn%20Object%20Reference) (BP_PSS :type BP%20PSS%20Object%20Reference))
  (return false))