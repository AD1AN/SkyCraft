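; BP_ShakingTree is a tree resource actor that shakes when its HealthSystem reports damage.
; The first hit caches the actor's rotation, and every hit restarts the Shaking timeline from the beginning.
; The timeline curve blends from the cached rotation toward a slight roll at the same yaw using teleport rotation, then restores the original rotation when finished.
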(event OnDamage(HealthSystem)
  (params (DamageGlobalType :type EDamageGlobalType%20Enum :default "Slash") (DA_Item :type Data%20Asset%20Object%20Reference) (DamageRatio :type Float%20%28single-precision%29) (HitLocation :type Vector :default "0, 0, 0"))
  (if (Variables|Default|GethaveRotation)
    (bind _newtrack_0 (Timeline|Shaking PlayFromStart)
      (:Update
        (Transformation|SetActorRotation (Math|Rotator|Lerp(Rotator) (Variables|Default|GetInitialRotation) (Math|Rotator|MakeRotator 1.0 0.0 (.yaw (Variables|Default|GetInitialRotation))) _newtrack_0) true))
      (:Finished
        (Transformation|SetActorRotation (Variables|Default|GetInitialRotation) true)))
    (else
      (Variables|Default|SetInitialRotation (Transformation|GetActorRotation))
      (Variables|Default|SethaveRotation true)
      (Timeline|Shaking PlayFromStart))))

(fn ConstructionScript)