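; BP_FallingTree is a tree resource that leaves a stump and a falling log when its health runs out.
; On death, the server asks the game systems reached through its Island to spawn a Grimroot stump resource at the tree's local location and rotation.
; It also spawns a BP_FallingLog, attaches it to the Island using island-relative coordinates, and gives it a random angular impulse so it topples.
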(event OnDie(HealthComponent)
  (bind _rootcomponent (Variables|Transformation|GetRootComponent))
  (bind _island (Variables|Default|GetIsland))
  (bind _relativelocation (Variables|/Script/Engine.SceneComponent|GetRelativeLocation _rootcomponent))
  (Networking|SwitchHasAuthority
    (:Authority
      (Class|GMS|SpawnResource (Variables|/Script/SkyCraft.GSS|GetGMS (Variables|/Script/SkyCraft.Island|GetGSS _island)) _island _relativelocation (Variables|/Script/Engine.SceneComponent|GetRelativeRotation _rootcomponent) "/Game/DataAssets/Resource/R_GrimrootStump.R_GrimrootStump" 0 false 0)
      (bind _returnvalue (Game|SpawnActorfromClass "/Game/Blueprints/BP_FallingLog.BP_FallingLog_C" (Math|Transform|MakeTransform _relativelocation "0, 0, 0" "1.000000,1.000000,1.000000") "AlwaysSpawn" "MultiplyWithRoot" 0 0))
      (Transformation|AttachActorToActor _returnvalue (Variables|Default|GetIsland) "None" "KeepRelative" "KeepRelative" "KeepRelative" true)
      (Class|PrimitiveComponent|AddAngularImpulseinDegrees (Variables|/Game/Blueprints/BP_FallingLog.BP_FallingLog_C|GetStaticMesh _returnvalue) (* (Math|Random|RandomUnitVector) 1e+01) "None" true))))

(event EventBeginPlay)

(fn ConstructionScript)